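; Newspaper save point that opens a save widget on interaction, passing itself as a reference and freezing interaction while input is UI-only.
; Its Cinematic event fades through black, hides the HUD, plays a sequencer cinematic, moves the player to a spawn transform and calls Save.
; Sequence end restores the HUD and interaction, while a separate end-interact event just restores game input and interaction.
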(event `self.InteractableComponent.OnInteract`
  (bind _returnvalue (`GameplayStatics.GetPlayerController` 0))
  ;[1 1 1 0.33] Interaction
  (`self.SetInteractionFreezed` true)
  (bind _widget (`/Game/Design/Widgets/WBP_Viewport.PushWidgetSimple` (`/Game/Design/_GameManagement/Core/BP_MetroHUD.Viewport` (cast `/Game/Design/_GameManagement/Core/BP_MetroHUD` (`PlayerController.GetHUD` _returnvalue) :!pure true)) "/Game/Design/Widgets/MainMenu/WBPC_Save.WBPC_Save_C"))
  (bind _aswbpc_save (cast `/Game/Design/Widgets/MainMenu/WBPC_Save` _widget))
  (set `/Game/Design/Widgets/MainMenu/WBPC_Save.Newspaper Ref` self _aswbpc_save)
  (`WidgetBlueprintLibrary.SetInputMode_UIOnlyEx` _returnvalue _aswbpc_save))

(event `Cinematic`
  ;[1 1 1 0.33] Fade in-out
  (`self.Fade` 1.0 true)
  (`KismetSystemLibrary.Delay` 1.0)
  (`self.Fade` 0.0)
  ;[1 1 1 0.33] Hide HUD
  (bind _asmain_hud (cast `MainHUD` (`PlayerController.GetHUD` (`GameplayStatics.GetPlayerController` 0))))
  (`MainHUD.SetUIMode` _asmain_hud true)
  ;[1 1 1 0.33] Trigger cinematic
  (`self.PlaySaveCinematic`)
  (`WidgetBlueprintLibrary.SetInputMode_GameOnly` (`GameplayStatics.GetPlayerController` 0)))

(event `PlaySaveCinematic`
  (bind (_returnvalue_location _returnvalue_rotation) (`KismetMathLibrary.BreakTransform` (`self.GetTransform` (`self.SpawnPlayerStart`))))
  ;[1 1 1 0.33] Play Cinematic (SEQUENCER CINEMATIC COMPONENT)
  (`/Game/Design/EnvironmentEvents/Components/BP_TriggerEventReceiver_Component.OnPlayComponentSpecificEvent` (`self.SequencerCinematic`) false null)
  ;[1 1 1 0.33] Set new Player's Transform
  (`self.K2_SetActorLocationAndRotation` :`self` (`GameplayStatics.GetPlayerCharacter` 0) :`NewLocation` _returnvalue_location)
  (`Controller.SetControlRotation` (`GameplayStatics.GetPlayerController` 0) _returnvalue_rotation)
  (`self.Save`))

(event `self.SequencerCinematic.OnSequenceEnd`
  ;[1 1 1 0.33] Restore HUD
  (bind _asmain_hud (cast `MainHUD` (`PlayerController.GetHUD` (`GameplayStatics.GetPlayerController` 0))))
  (`MainHUD.SetUIMode` _asmain_hud false)
  (`self.Fade` 1.0)
  (`self.SetInteractionFreezed` false))

(event `End Intercat`
  (`WidgetBlueprintLibrary.SetInputMode_GameOnly` (`GameplayStatics.GetPlayerController` 0))
  (`self.SetInteractionFreezed` false))

(fn `Fade`
  (params (Time :type "Float (single-precision)") (bIsFadeIn :type Boolean))
  (`/Game/Design/Widgets/WBP_BlackFader.Fade` (`/Game/Design/Widgets/WBP_Viewport.BlackFader` (`/Game/Design/_GameManagement/Core/BP_MetroHUD.Viewport` (cast `/Game/Design/_GameManagement/Core/BP_MetroHUD` (`PlayerController.GetHUD` (`GameplayStatics.GetPlayerController` 0)) :!pure true))) Time bIsFadeIn))

(fn `UserConstructionScript`)