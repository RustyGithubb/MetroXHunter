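; BP_LifeComponent is a component that tracks an actor's health and death state, starting at max life.
; GetHit ignores dead owners, otherwise subtracts damage, prints a debug string and broadcasts health update, hit direction and, at zero or below, death.
; GetHeal clamps life to the maximum, while ResetLife and SetLifeToValue overwrite it and update the dead flag.
; All changes after BeginPlay notify listeners through event dispatchers.
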(event `self.ReceiveBeginPlay`
  ;[1 0 0.01418 0.33] BEGINPLAY
  ;;[0 1 0.4761] Set CurrentLife
  (set `self.CurrentLife` (`self.MaxLife`)))

(fn `GetHeal`
  (params (HealAmount :type Integer))
  (set `self.CurrentLife` (`KismetMathLibrary.Clamp` (+ (`self.CurrentLife`) HealAmount) 0 (`self.MaxLife`)))
  (`self.OnHealthUpdate`))

(fn `GetHit`
  (params (DamageAmount :type Integer) (ImpactDirection :type "Vector Structure"))
  (if (not (`self.IsDead`))
    (`KismetSystemLibrary.PrintString` (`KismetStringLibrary.Concat_StrStr` (`KismetStringLibrary.Conv_IntToString` DamageAmount) " Damage on" (`KismetSystemLibrary.GetDisplayName` (`self.GetOwner`))))
    (set `self.CurrentLife` (- (`self.CurrentLife`) DamageAmount))
    (`self.OnHealthUpdate`)
    (`self.OnHit` (`local.ImpactDirection`))
    ;[0 1 0.6778] Call OnDeath event
    (if (<= (`self.CurrentLife`) 0)
      (set `self.IsDead` true)
      (`self.OnDeath`))))

(fn `ResetLife`
  (set `self.CurrentLife` (`self.MaxLife`))
  (set `self.IsDead` false)
  (`self.OnHealthUpdate`))

(fn `SetLifeToValue`
  (params (NewLifeValue :type Integer))
  (set `self.CurrentLife` NewLifeValue)
  (`self.OnHealthUpdate`)
  (if (> (`self.CurrentLife`) 0)
    (set `self.IsDead` false)
    (else
      (set `self.IsDead` true)
      (`self.OnDeath`))))