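; Electrical generator gameplay-element actor with visual effects that react to damage and death through its Health component.
; On damage it spawns a jittering lightning ball at LightningsPoint, activates GeneratorExplosion, then destroys the ball after a short delay.
; On death it only activates GeneratorExplosion.
; The LightningElectricity activation nodes are unconnected and never run, and the construction script is empty.
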(event `self.Health.OnDeath`
  (params (DamageContext :type "DamageContext Structure (by ref)"))
  (`ActorComponent.Activate` (`self.Generator_Explosion`) false))

(event `self.Health.OnDamage`
  (params (DamageContext :type "DamageContext Structure (by ref)"))
  (bind _returnvalue (`|SpawnActorFromClass` "/Game/Art/VFX/GPE/Lightnings/BP_Lightning_Ball_Jitter_GPE.BP_Lightning_Ball_Jitter_GPE_C" (`SceneComponent.K2_GetComponentToWorld` (`self.Lightnings_Point`)) "Undefined" "MultiplyWithRoot" null null))
  (`ActorComponent.Activate` (`self.Generator_Explosion`) false)
  (`KismetSystemLibrary.Delay` 1.0)
  (`self.K2_DestroyActor` _returnvalue))

(fn `UserConstructionScript`)