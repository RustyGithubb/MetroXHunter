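; Destructible fire extinguisher that turns into a leaking, physics-driven projectile when its Health component dies, then bursts.
; Death attaches leak smoke at the impact, applies an upward-biased impulse and random spin, then a Timeline applies thrust against the stored local hit normal until explosion effects and destruction.
; Its first Hit event plays a fall sound and writes the NOTRE_DAME achievement, granting METRO when the game instance's unlock count reaches the total.
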(event `self.Health.OnDeath`
  (params (DamageContext :type "DamageContext Structure (by ref)"))
  (bind _returnvalue (`KismetMathLibrary.RandomFloatInRange` -10000.0 10000.0))
  (bind _sm_fire_extinguisher (`self.SM_Fire_Extinguisher`))
  (bind (_bblockinghit _binitialoverlap _time _distance _location _impactpoint _normal _impactnormal _physmat _hitactor _hitcomponent _hitbonename _bonename _hititem _elementindex _faceindex _tracestart _traceend) (`GameplayStatics.BreakHitResult` (`.HitResult` (break `DamageContext` DamageContext))))
  (set `self.LocalHitDirection` (`KismetMathLibrary.InverseTransformDirection` (`self.GetTransform`) (`KismetMathLibrary.NegateVector` _impactnormal)))
  (`NiagaraFunctionLibrary.SpawnSystemAttached` "/Game/Art/VFX/NS_Smoke/NS_Smoke_FireExtinguisher_Leak.NS_Smoke_FireExtinguisher_Leak" (`self.SM_Fire_Extinguisher`) "None" _location (`KismetMathLibrary.Conv_VectorToRotator` _impactnormal) "KeepWorldPosition")
  (`PrimitiveComponent.SetSimulatePhysics` (`self.SM_Fire_Extinguisher`) true)
  (`PrimitiveComponent.AddImpulse` _sm_fire_extinguisher (* (`KismetMathLibrary.Vector_SlerpNormals` (`KismetMathLibrary.GetDirectionUnitVector` _tracestart _traceend) (`KismetMathLibrary.Vector_Up`) (`KismetMathLibrary.RandomFloatInRange` 0.5 0.75)) 500000.0) "None" false)
  (`PrimitiveComponent.AddTorqueInDegrees` _sm_fire_extinguisher (`KismetMathLibrary.MakeVector` _returnvalue 0.0 _returnvalue) "None" true)
  (`Timeline|Timeline` :!via `PlayFromStart`
    (:`Update`
      (`PrimitiveComponent.AddForce` (`self.SM_Fire_Extinguisher`) (* (`KismetMathLibrary.TransformDirection` (`self.GetTransform`) (`self.LocalHitDirection`)) 1000.0) "None" true))
    (:`Finished`
      (`NiagaraFunctionLibrary.SpawnSystemAtLocation` "/Game/Art/VFX/NS_Smoke/NS_Smoke_FireExtinguisher_Exploding.NS_Smoke_FireExtinguisher_Exploding" (`KismetSystemLibrary.GetComponentBounds` (`self.SM_Fire_Extinguisher`)))
      (`GameplayStatics.SpawnSound2D` "/Game/Sounds/Audio/SD/SoundWaves/GPE/Extinguisher/SW_GPE_Extinguisher_Explosion.SW_GPE_Extinguisher_Explosion" 1.0 1.0 0.0 null)
      (`self.K2_DestroyActor`))))

(event `self.ReceiveHit`
  (params (MyComp :type "PrimitiveComponent Object Reference") (Other :type "Actor Object Reference") (OtherComp :type "PrimitiveComponent Object Reference") (bSelfMoved :type Boolean) (HitLocation :type "Vector Structure") (HitNormal :type "Vector Structure") (NormalImpulse :type "Vector Structure") (Hit :type "HitResult Structure (by ref)"))
  (bind _returnvalue (`GameplayStatics.GetPlayerController` 0))
  (bind _returnvalue_2 (`GameplayStatics.GetPlayerController` 0))
  (`/Engine/EditorBlueprintResources/StandardMacros.DoOnce` false
    (:`Completed`
      (`GameplayStatics.SpawnSound2D` "/Game/Sounds/Audio/SD/SoundWaves/GPE/Extinguisher/SW_GPE_Extinguisher_FallDown_01.SW_GPE_Extinguisher_FallDown_01" 1.0 1.0 0.0 null)
      ;[0 1 0.8336 0.33] ACHIEVEMENT : NOTRE_DAME
      (`AchievementQueryCallbackProxy.CacheAchievements` _returnvalue_2
        (:`OnSuccess`
          (bind (_bfoundid _progress) (`AchievementBlueprintLibrary.GetCachedAchievementProgress` _returnvalue_2 "NOTRE_DAME"))
          (if _bfoundid
            (if (> _progress 0.0)
              (`KismetSystemLibrary.PrintString` "Achievements already unlocked !" true true (struct :`G` 1.0 :`B` 0.012183 :`A` 1.0) 6.0)
              (else
                (`AchievementWriteCallbackProxy.WriteAchievementProgress` _returnvalue_2 "NOTRE_DAME"
                  (:`OnSuccess`
                    (`KismetSystemLibrary.PrintString` "Achievement unlocked !" true true (struct :`G` 1.0 :`B` 0.96591 :`A` 1.0) 6.0)
                    (bind _asbp_metro_game_instance (cast `/Game/Design/_GameManagement/Core/BP_MetroGameInstance` (`GameplayStatics.GetGameInstance`)))
                    (set `/Game/Design/_GameManagement/Core/BP_MetroGameInstance.AchievementsUnlocked` (+ (`/Game/Design/_GameManagement/Core/BP_MetroGameInstance.AchievementsUnlocked` _asbp_metro_game_instance) 1) _asbp_metro_game_instance)
                    (if (== (`/Game/Design/_GameManagement/Core/BP_MetroGameInstance.AchievementsUnlocked` _asbp_metro_game_instance) (`/Game/Design/_GameManagement/Core/BP_MetroGameInstance.TotalNormalAchievements` _asbp_metro_game_instance))
                      (bind (_bfoundid_2 _progress_2) (`AchievementBlueprintLibrary.GetCachedAchievementProgress` _returnvalue "METRO"))
                      (if _bfoundid_2
                        (if (> _progress_2 0.0)
                          (`KismetSystemLibrary.PrintString` "Achievements already unlocked !" true true (struct :`G` 1.0 :`B` 0.012183 :`A` 1.0) 10.0)
                          (else
                            (`AchievementWriteCallbackProxy.WriteAchievementProgress` _returnvalue "METRO")))
                        (else
                          (`KismetSystemLibrary.PrintString` "Didn't find ID" true true (struct :`R` 1.0 :`G` 0.408724 :`A` 1.0) 10.0))))))))
            (else
              (`KismetSystemLibrary.PrintString` "Didn't find ID" true true (struct :`R` 1.0 :`G` 0.408724 :`A` 1.0) 6.0))))
        (:`OnFailure`
          (`KismetSystemLibrary.PrintString` "Couldn't cache achievements !" true true (struct :`R` 1.0 :`A` 1.0) 6.0))))))

(fn `UserConstructionScript`)