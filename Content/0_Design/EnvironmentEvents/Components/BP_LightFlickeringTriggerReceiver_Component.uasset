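; Trigger receiver component that flickers the lights on a list of actors when its trigger event fires.
; On BeginPlay it caches each Light Component's starting intensity, plus an optional random time offset to desync them.
; Once triggered, Tick scales those intensities by a float curve, using dilation-adjusted time wrapped by modulo.
; It loops forever or stops at the curve's end, restoring the lights or switching them off.
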(event `self.ReceiveBeginPlay`
  (`self.SetComponentTickEnabled` false)
  (if (`KismetArrayLibrary.Array_IsNotEmpty` (`self.ActorsThatShouldFlicker`))
    (bind _flickeringcurve (`self.FlickeringCurve`)
      (:`then`
        (set `self.MaxFlickerTime` (`.MaxTime` (`CurveBase.GetTimeRange` _flickeringcurve)))
        (`self.RegisterAllLightsAndDefaultBrightnesses`))
      (:`else`
        ;[0.0625 0.001432 0 0.33] ERROR PRINT
        (`KismetSystemLibrary.PrintText` (`|FormatText` "LightFlickeringComponent on Actor {actorName} \nhas not been given a CurveFloat to follow. \nPlease Add one." (`KismetSystemLibrary.GetDisplayName` (`self.GetOwner`))))))))

(event `self.ReceiveTick`
  (params (DeltaSeconds :type "Float (single-precision)"))
  ;[0.1573 0.05425 0.2604 0.33] Take SlowMo into account
  (`/Game/o_Libraries/BPL_GeneralUtilities.Increase Value Float` (`self.CurrentFlickerTime`) (* (`GameplayStatics.GetWorldDeltaSeconds`) (`GameplayStatics.GetGlobalTimeDilation`)))
  ;[0.06606 0.1828 0.2031 0.33] Should we stop the flickering yet?
  (if (and (not (`self.PlayInfinite`)) (>= (`self.CurrentFlickerTime`) (`self.MaxFlickerTime`)))
    (`self.StopFlickering`)
    (else
      (`self.UpdateAllLights`))))

(fn `OnPlayComponentSpecificEvent`
  (params (FromBoxEnter :type Boolean))
  (`self.SetComponentTickEnabled` true))

(fn `RegisterAllLightsAndDefaultBrightnesses`
  (locals (CurrentlyEvaluatedLights :type "Array of LightComponent Object Reference"))
  (`KismetArrayLibrary.Array_Clear` (`self.CustomLightOffsets`))
  (`KismetArrayLibrary.Array_Clear` (`self.LightsToFlicker`))
  (`KismetArrayLibrary.Array_Clear` (`self.StartingLightIntensities`))
  ;[0.1724 0.05414 0.1771 0.33] Loop through all given Actors and get all of their Lights (if they have any!!)
  (for _array_element (`self.ActorsThatShouldFlicker`)
    (bind _output_get (set `local.CurrentlyEvaluatedLights` (`Actor.K2_GetComponentsByClass` _array_element "/Script/Engine.LightComponent")))
    (if (`KismetArrayLibrary.Array_IsNotEmpty` _output_get)
      ;[0.1979 0.08918 0.04725 0.33] Register each Light with their Starting Intensity, and if needed, a Custom Time Offset to desync them all.
      (for _array_element_2 (`local.CurrentlyEvaluatedLights`)
        (`KismetArrayLibrary.Array_Add` (`self.LightsToFlicker`) _array_element_2)
        (`KismetArrayLibrary.Array_Add` (`self.StartingLightIntensities`) (`LightComponentBase.Intensity` _array_element_2))
        (if (`self.RandomlyOffsetLights`)
          (`KismetArrayLibrary.Array_Add` (`self.CustomLightOffsets`) (`KismetMathLibrary.RandomFloatInRange` 0.0 (`self.MaxFlickerTime`)))))
      (else
        ;[0.1927 0 0 0.33] ERROR PRINT
        (`KismetSystemLibrary.PrintText` (`|FormatText` "LightFlickeringComponent on Actor {actorName} \nhas been given Actor {fakeLight}, but this Actor doesn't have any Light Components. \nPlease remove the Actor or add a Light to it." (`KismetSystemLibrary.GetDisplayName` (`self.GetOwner`)) (`KismetSystemLibrary.GetDisplayName` _array_element)))))))

(fn `StopFlickering`
  (`self.SetComponentTickEnabled` false)
  ;[0.09668 0.1593 0.2812 0.33] Why use an If Branch and not a Select Float?
  ; Because Select nodes evaluate both possibilities before checking the condition (that's why they can give NullReferenceExceptions even if that wouldn't have been the outcome)
  ; So we avoid bothering the Array by doing a simple If-Else.
  ; Then we do the Branch before the Foreach because there's no need of checking the boolean 40 times
  ; Yes the code is visually a bit redundant, but it's more effective
  ; Fight me <3
  (if (`self.EndWithTurnOff`)
    (for _array_element (`self.LightsToFlicker`)
      (`LightComponent.SetIntensity` _array_element 0.0))
    (else
      (for (_array_element_2 _array_index) (`self.LightsToFlicker`)
        (`LightComponent.SetIntensity` _array_element_2 (`|GetArrayItem` (`self.StartingLightIntensities`) _array_index))))))

(fn `UpdateAllLights`
  (locals (CurrentLight :type "LightComponent Object Reference") (CurrentArrayIndex :type Integer))
  ;[0.02121 0.08333 0.04914 0.33] Why use an If Branch and not a Select Float?
  ; Because Select nodes evaluate both possibilities before checking the condition.
  ; But in this case, if we don't RandomlyOffsetLights, CustomLightOffsets is an empty array, so evaluating this output would create an Error: we can't access an index that doesn't exist.
  ;
  ; Then we do the Branch before the Foreach because there's no need of checking the boolean 40 times
  ; Yes the code is visually a bit redundant, but it's more effective
  ; Fight me <3
  (if (`self.RandomlyOffsetLights`)
    (for (_array_element _array_index) (`self.LightsToFlicker`)
      (set `local.CurrentLight` _array_element)
      (set `local.CurrentArrayIndex` _array_index)
      (`LightComponent.SetIntensity` (`local.CurrentLight`) (* (`CurveFloat.GetFloatValue` (`self.FlickeringCurve`) (mod (+ (`|GetArrayItem` (`self.CustomLightOffsets`) (`local.CurrentArrayIndex`)) (`self.CurrentFlickerTime`)) (`self.MaxFlickerTime`))) (`|GetArrayItem` (`self.StartingLightIntensities`) (`local.CurrentArrayIndex`)))))
    (else
      (for (_array_element_2 _array_index_2) (`self.LightsToFlicker`)
        (set `local.CurrentLight` _array_element_2)
        (set `local.CurrentArrayIndex` _array_index_2)
        (`LightComponent.SetIntensity` (`local.CurrentLight`) (* (`CurveFloat.GetFloatValue` (`self.FlickeringCurve`) (mod (`self.CurrentFlickerTime`) (`self.MaxFlickerTime`))) (`|GetArrayItem` (`self.StartingLightIntensities`) (`local.CurrentArrayIndex`))))))))