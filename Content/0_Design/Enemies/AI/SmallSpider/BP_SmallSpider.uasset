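; Small spider enemy with a cooldown-limited jump attack that deals melee damage through a trigger disabled on landing.
; Any weak point death kills it into a ragdoll, pushed back by bullets, with a chance to start a delayed shriek.
; The shriek changes its material and can be stopped by depleting a separate life component.
; Otherwise it alerts shuffled receiver components in radius, capping limit-counted ones at a random number.
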(event `self.ReceiveBeginPlay`
  ;[1 1 1 0.25] BEGIN PLAY
  (`parent.ReceiveBeginPlay`)
  ;;[1 1 1 0.33] Bind WeakPoint's LifeComponent Event OnDeath
  (for _array_element (`self.WeakPoints`)
    (add `/Game/0_Design/LifeSystem/BP_LifeComponent.OnDeath` (`/Game/0_Design/EyeVisionSystem/BP_WeakPoints.LifeComponent` _array_element) (delegate `OnWeakPointDeath`)))
  (set `self.MeshMaterial` (`PrimitiveComponent.GetMaterial` (`self.Mesh`) 0)))

(event `OnWeakPointDeath`
  (params (DamageContext :type "/Game/0_Design/LifeSystem/Structs/F_DamageContext Structure"))
  ;[1 1 1 0.25] BEGIN PLAY
  (`self.Kill` (select `/Game/0_Design/LifeSystem/Enums/E_DamageType` DamageContext_DamageType_28_5E2C43D64100A842568DC98F4D5179BC :`NewEnumerator0` (`self.K2_GetActorLocation` DamageContext_AttackerActor_23_F38EDFB541911B9E1D34B48BF85F0DB0)))
  (`ActorComponent.Activate` (`self.FXBlood`) true))

(event `self.ReceiveTick`
  (params (DeltaSeconds :type "Float (single-precision)"))
  (`parent.ReceiveTick` DeltaSeconds)
  (set `self.CurrentAttackJumpCooldown` (- (`self.CurrentAttackJumpCooldown`) DeltaSeconds))
  (`self.UpdateMovementSound`))

(event `self.BP_LifeComponent_Shriek.OnDeath`
  (params (DamageContext :type "/Game/0_Design/LifeSystem/Structs/F_DamageContext Structure"))
  (bind _mesh (`self.Mesh`))
  (if (`self.bIsShrieking`)
    (`self.StopShriek`)
    (if (`SceneComponent.IsSimulatingPhysics` _mesh "None")
      (`SkeletalMeshComponent.AddImpulseToAllBodiesBelow` _mesh (`self.ComputeKnockbackFrom` (`self.K2_GetActorLocation` DamageContext_AttackerActor_23_F38EDFB541911B9E1D34B48BF85F0DB0)) "None" false true))))

(event `self.DamageTrigger.OnComponentBeginOverlap`
  (params (OverlappedComponent :type "PrimitiveComponent Object Reference") (OtherActor :type "Actor Object Reference") (OtherComp :type "PrimitiveComponent Object Reference") (OtherBodyIndex :type Integer) (bFromSweep :type Boolean) (SweepResult :type "HitResult Structure (by ref)"))
  (bind _returnvalue (`self.GetComponentByClass` OtherActor "/Game/0_Design/LifeSystem/BP_LifeComponent.BP_LifeComponent_C"))
  (if (!= self OtherActor)
    ;[1 1 1 0.33] Double-Check it's not a Spider
    (if (not (`.bSuccess` (cast `/Game/0_Design/EyeVisionSystem/BP_WeakPoints` OtherActor :!pure true)))
      (`/Engine/EditorBlueprintResources/StandardMacros.IsValid` _returnvalue
        (:`Is Valid`
          (`/Game/0_Design/LifeSystem/BP_LifeComponent.TakeDamage` _returnvalue (make `/Game/0_Design/LifeSystem/Structs/F_DamageContext` (`self.AttackJumpDamage`) "NewEnumerator4" self self SweepResult)))))))

(event `self.OnLanded`
  (params (Hit :type "HitResult Structure (by ref)"))
  (`PrimitiveComponent.SetCollisionEnabled` (`self.DamageTrigger`) "NoCollision"))

(event `self.BP_LifeComponent_Shriek.OnDamage`
  (params (DamageContext :type "/Game/0_Design/LifeSystem/Structs/F_DamageContext Structure"))
  (`ActorComponent.Activate` (`self.FXBlood`) true))

(fn `ApplyTimeBeforeDestroy`
  (`self.SetLifeSpan` (`self.TimeBeforeDestroy`)))

(fn `ComputeKnockbackFrom`
  (params (Location :type "Vector Structure"))
  (returns (Knockback :type "Vector Structure"))
  (return (* (`KismetMathLibrary.GetDirectionUnitVector` Location (`self.K2_GetActorLocation`)) 10.0)))

(fn `DoAttackJump`
  (`self.LaunchCharacter` (* (`KismetMathLibrary.Vector_SlerpNormals` (`KismetMathLibrary.Vector_Up`) (`self.GetActorForwardVector`) (`self.AttackJumpUpForwardRatio`)) (`self.AttackJumpForce`)))
  (set `self.CurrentAttackJumpCooldown` (`self.AttackJumpCooldown`))
  (`PrimitiveComponent.SetCollisionEnabled` (`self.DamageTrigger`) "QueryOnly")
  (`/EventDispatcherHub/FunctionLibrary/BPL_EventDispatcherHub.Call Single Gameplay Event` (struct :`TagName` "Event.SmallSpider.OnAttackJump") self))

(fn `DoShriek`
  (locals (ShriekReceiver :type "/Game/0_Design/Enemies/Shriek/BP_ShriekReceiverComponent Object Reference") (RemainingToBroadcast :type Integer :default 0))
  (bind _shriekradius (`self.ShriekRadius`))
  (bind _shriekmaxemitcountrange (`self.ShriekMaxEmitCountRange`))
  (bind _remainingtobroadcast (`local.RemainingToBroadcast`))
  (`self.OnShriek` self)
  (`self.StopShriek`)
  (set `local.RemainingToBroadcast` (`KismetMathLibrary.RandomIntegerInRange` (`.Value` (break `Int32RangeBound` (break `Int32Range` _shriekmaxemitcountrange))) (`.Value` (break `Int32RangeBound` (`.UpperBound` (break `Int32Range` _shriekmaxemitcountrange))))))
  ;[1 1 1 0.33] Emit Shriek
  (bind _outactors (`KismetSystemLibrary.SphereOverlapActors` (`self.K2_GetActorLocation`) _shriekradius (`|MakeArray` "ObjectTypeQuery2" "ObjectTypeQuery7" "ObjectTypeQuery3" :!type "EObjectTypeQuery Enum")))
  (`KismetArrayLibrary.Array_Shuffle` _outactors)
  (for _array_element _outactors
    (bind _output_get (set `local.ShriekReceiver` (`self.GetComponentByClass` _array_element "/Game/0_Design/Enemies/Shriek/BP_ShriekReceiverComponent.BP_ShriekReceiverComponent_C")))
    (`/Engine/EditorBlueprintResources/StandardMacros.IsValid` _output_get
      (:`Is Valid`
        (if (`/Game/0_Design/Enemies/Shriek/BP_ShriekReceiverComponent.IsReceivingCountAsLimit` _output_get)
          (if (> _remainingtobroadcast 0)
            (`/Engine/EditorBlueprintResources/StandardMacros.DecrementInt` _remainingtobroadcast
              (:`  `
                (bind _canreceive (`/Game/0_Design/Enemies/Shriek/BP_ShriekReceiverComponent.CanReceive` _output_get self :!label _label))
                (if _canreceive
                  (`/Game/0_Design/Enemies/Shriek/BP_ShriekReceiverComponent.ReceiveShriek` _output_get (make `/Game/0_Design/Enemies/Shriek/F_ShriekEmissionContext` self (`self.K2_GetActorLocation` self) _shriekradius))))))
          (else
            (goto _label))))))
  (`GameplayStatics.PlaySoundAtLocation` "/Game/4_Sounds/Placeholders/SculkShriekers/SC_CreatureShriek.SC_CreatureShriek" (`SceneComponent.K2_GetComponentLocation` (`self.Mesh`)) (`self.K2_GetActorRotation`) 0.5 (`KismetMathLibrary.RandomFloatInRange` 0.9 1.1) 0.0 null null self null))

(fn `IsAttackJumpOnCooldown`
  (returns (IsOnCooldown :type Boolean))
  (return (> (`self.CurrentAttackJumpCooldown`) 0.0)))

(fn `Kill`
  (params (ImpactLocation :type "Vector Structure"))
  (bind _mesh (`self.Mesh`))
  (set `self.bIsDead` true)
  ;[1 1 1 0.33] Enable ragdoll
  (`PrimitiveComponent.SetSimulatePhysics` _mesh true)
  (`PrimitiveComponent.SetCollisionProfileName` _mesh "Ragdoll" true)
  ;[1 1 1 0.33] Impulse the ragdoll w/ shoot force
  (if (not (`KismetMathLibrary.Vector_IsNearlyZero` ImpactLocation))
    (`SkeletalMeshComponent.AddImpulseToAllBodiesBelow` (`self.Mesh`) (`self.ComputeKnockbackFrom` ImpactLocation) "None" false true))
  ;[1 1 1 0.33] Disable collision
  (`PrimitiveComponent.SetCollisionEnabled` (`self.CapsuleComponent`) "NoCollision")
  (`PrimitiveComponent.SetCollisionEnabled` (`self.DamageTrigger`) "NoCollision")
  (`self.OnDeath`)
  (`/EventDispatcherHub/FunctionLibrary/BPL_EventDispatcherHub.Call Single Gameplay Event` (struct :`TagName` "Event.SmallSpider.Death") self)
  (bind _isshrieking (`self.TryShriek`))
  (if (not _isshrieking)
    (`self.ApplyTimeBeforeDestroy`)))

(fn `StartShriek`
  (set `self.bIsShrieking` true)
  ;[1 1 1 0.33] Visual indicator
  (`PrimitiveComponent.SetMaterial` (`self.Mesh`) 0 "/Game/1_Art/MaterialLibrary/DebugMaterials/MI_SmallSpider_Shriek.MI_SmallSpider_Shriek")
  ;[1 1 1 0.33] Delay shriek
  (bind _returnvalue (`KismetSystemLibrary.K2_SetTimer` null "DoShriek" (`self.ShriekTime`)))
  (set `self.ShriekTimer` _returnvalue)
  ;[1 1 1 0.33] If dead, shows the whole body as weak point
  (if (`self.bIsDead`)
    (`PrimitiveComponent.SetRenderCustomDepth` (`self.Mesh`) true))
  ;[1 1 1 0.33] Make it possible to stop the shriek
  (`/Game/0_Design/LifeSystem/BP_LifeComponent.ResetLife` (`self.BP_LifeComponent_Shriek`))
  (`self.OnShriekStateChanged` self true))

(fn `StopShriek`
  (bind _shriektimer (`self.ShriekTimer`))
  (bind _mesh (`self.Mesh`))
  (if (`KismetSystemLibrary.K2_IsValidTimerHandle` _shriektimer)
    (`KismetSystemLibrary.K2_ClearAndInvalidateTimerHandle` _shriektimer))
  (set `self.bIsShrieking` false)
  ;[1 1 1 0.33] Reset visual indicator
  (`PrimitiveComponent.SetMaterial` _mesh 0 (`self.MeshMaterial`))
  (`PrimitiveComponent.SetRenderCustomDepth` _mesh false)
  (`self.OnShriekStateChanged` self)
  (if (`self.bIsDead`)
    (`self.ApplyTimeBeforeDestroy`)))

(fn `TryShriek`
  (returns (IsShrieking :type Boolean))
  (if (not (`self.bIsShrieking`))
    ;[1 1 1 0.33] Shriek Chance
    (if (< (`KismetMathLibrary.RandomFloat`) (`self.ShriekProbability`))
      (`self.StartShriek`)
      (return true)
      (else
        _)))
  (return false))

(fn `UpdateMovementSound`
  (bind _charactermovement (`self.CharacterMovement`))
  (bind _movementaudio (`self.MovementAudio`))
  (if (and (not (`KismetMathLibrary.Vector_IsNearlyZero` (`CharacterMovementComponent.GetLastUpdateVelocity` _charactermovement))) (`NavMovementComponent.IsMovingOnGround` _charactermovement))
    (if (not (`AudioComponent.IsPlaying` _movementaudio))
      (`AudioComponent.Play` _movementaudio 0.0))
    (else
      (`AudioComponent.Stop` _movementaudio))))

(fn `UserConstructionScript`
  (`parent.UserConstructionScript`))