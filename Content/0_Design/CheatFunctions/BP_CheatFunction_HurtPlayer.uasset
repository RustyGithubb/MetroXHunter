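; Cheat function that hurts the player on demand, by a configurable HurtAmount.
; On init it waits one tick, then caches the BP_LifeComponent of the first player's pawn.
; When triggered it calls GetHit on that component with a hit info holding the damage and a random horizontal unit direction, so the damage goes through the life component's hit handling.
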(event `self.OnInit`
  (`KismetSystemLibrary.DelayUntilNextTick`)
  (set `self.PlayerLifeComponent` (`Actor.GetComponentByClass` (`GameplayStatics.GetPlayerPawn` 0) "/Game/0_Design/LifeSystem/BP_LifeComponent.BP_LifeComponent_C")))

(event `self.OnCheat`
  (`/Game/0_Design/LifeSystem/BP_LifeComponent.GetHit` (`self.PlayerLifeComponent`) (make `/Game/0_Design/LifeSystem/F_HitInfo` (`self.HurtAmount`) (`KismetMathLibrary.Vector_Normal2D` (`KismetMathLibrary.RandomUnitVector`)) "None" null null)))