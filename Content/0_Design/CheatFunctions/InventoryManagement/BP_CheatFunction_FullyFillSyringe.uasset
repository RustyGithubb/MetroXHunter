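; Cheat function that fully fills the player's healing syringe.
; On init it waits a tick, then caches the inventory component from the pawn controlled by the cheat manager's player controller.
; When the cheat runs, it calls the fill function on that cached component if it is valid.
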(event `self.OnInit`
  (`KismetSystemLibrary.DelayUntilNextTick`)
  (`self.RegisterInventoryComponent`))

(event `self.OnCheat`
  (bind _playerinventorycomponent (`self.PlayerInventoryComponent`)
    (:`then`
      (`/Game/0_Design/GameManagement_/BP_InventoryComponent.FullyFillHealingSyringe` _playerinventorycomponent))
    (:`else`)))

(fn `RegisterInventoryComponent`
  (set `self.PlayerInventoryComponent` (`Actor.GetComponentByClass` (`Controller.K2_GetPawn` (`CheatManager.GetPlayerController` (`self.CheatManager`))) "/Game/0_Design/GameManagement_/BP_InventoryComponent.BP_InventoryComponent_C")))