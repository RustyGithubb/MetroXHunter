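; BP_EyeVision detects which monster the player looks at while eye vision mode is active.
; Enter and quit events toggle the mode, and a throttled tick runs a long line trace from the player camera.
; A hit BP_BaseMonster becomes the current target and receives OnTargeted, while a miss or other hit clears it.
; Switching directly between monsters does not untarget the previous one.
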(event `self.ReceiveTick`
  (params (DeltaSeconds :type "Float (single-precision)"))
  ;[0.5052 0.008634 0 0.33] EVENT TICK ( 0.2s tick intervals)
  (if (`self.IsInEyeVision`)
    (`self.CheckForMonster`)))

(event `EnterEyeVision`
  ;[1 1 1 0.33] Enable / Disable EyeVision
  (set `self.IsInEyeVision` true))

(event `QuitEyeVision`
  ;[1 1 1 0.33] Enable / Disable EyeVision
  (set `self.IsInEyeVision` false))

(fn `CheckForMonster`
  (bind _playercamera (`self.PlayerCamera`))
  (bind _returnvalue (`SceneComponent.K2_GetComponentLocation` _playercamera))
  (bind (_outhit _returnvalue_2) (`KismetSystemLibrary.LineTraceSingle` :`Start` _returnvalue :`End` (+ (* (`SceneComponent.GetForwardVector` _playercamera) 30000) _returnvalue) :`TraceChannel` "TraceTypeQuery4" :`bTraceComplex` true :`TraceColor` (struct :`R` 1.0 :`G` 0.006403 :`A` 1.0) :`DrawTime` 3.0))
  ;[1 1 1 0.33] Check if hit something
  (if _returnvalue_2
    (bind (_bblockinghit _binitialoverlap _time _distance _location _impactpoint _normal _impactnormal _physmat _hitactor) (`GameplayStatics.BreakHitResult` _outhit))
    ;[1 1 1 0.33] Check if the hit isn't the current target
    (if (!= (`self.CurrentTarget`) _hitactor)
      ;[1 1 1 0.33] Set Current Target
      (bind _asbp_base_monster (cast `/Game/9_ShootingRange/Blueprints/BP_BaseMonster` _hitactor)
        (:`then`
          (bind _output_get (set `self.CurrentTarget` _asbp_base_monster))
          (`/Game/9_ShootingRange/Blueprints/BP_BaseMonster.OnTargeted` _output_get true (`self.PlayerCamera`)))
        (:`CastFailed`
          ;[1 1 1 0.33] Reset Current Target
          (bind _currenttarget (`self.CurrentTarget` :!label _label)
            (:`then`
              (`/Game/9_ShootingRange/Blueprints/BP_BaseMonster.OnTargeted` _currenttarget false null)
              (set `self.CurrentTarget` null))
            (:`else`)))))
    (else
      (goto _label))))