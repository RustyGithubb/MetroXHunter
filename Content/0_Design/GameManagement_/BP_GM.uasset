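; BP_GM is a Game Mode Blueprint that customizes where players spawn by overriding ChoosePlayerStart.
; A PlayerStartPIE actor takes priority, which supports Play From Here in the editor.
; Otherwise it picks the first PlayerStart tagged None or Start, and falls back to the parent implementation when none matches.
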(fn `ChoosePlayerStart`
  (params (Player :type "Controller Object Reference"))
  (returns (ReturnValue :type "Actor Object Reference"))
  ;[1 1 1 0.33] Support for 'Play From Here'
  (bind _returnvalue (`GameplayStatics.GetActorOfClass` "/Script/Engine.PlayerStartPIE"))
  (`/Engine/EditorBlueprintResources/StandardMacros.IsValid` _returnvalue
    (:`Is Valid`
      (return _returnvalue))
    (:`Is Not Valid`
      ;[1 1 1 0.33] Prioritize PlayerStarts with tags "None" or "Start"
      (bind _outactors (`GameplayStatics.GetAllActorsOfClass` "/Script/Engine.PlayerStart"))
      (for _array_element _outactors
        (bind _playerstarttag (`PlayerStart.PlayerStartTag` _array_element))
        (if (or (== _playerstarttag "None") (== _playerstarttag "Start"))
          (return _array_element)))
      (bind _returnvalue_2 (`parent.ChoosePlayerStart` Player))
      (return _returnvalue_2))))

(fn `UserConstructionScript`)