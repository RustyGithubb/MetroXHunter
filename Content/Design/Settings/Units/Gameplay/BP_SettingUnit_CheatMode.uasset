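; BP_SettingUnit_CheatMode is a boolean setting unit that toggles cheat input in the game.
; On initialize it defaults to on when running within the editor and off otherwise.
; When applied in game, it adds or removes the IMC_Cheat Enhanced Input mapping context for the first player controller, according to its value.
; This only happens if that controller has a valid CheatManager.
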(event `self.OnInitialize`
  (if (`UtilityLibrary.IsWithinEditor`)
    (set `self.bDefaultValue` true)
    (else
      (set `self.bDefaultValue` false))))

(event `self.OnApplySetting`
  (params (bInGame :type Boolean))
  (bind _returnvalue (pcsubsystem `EnhancedInputLocalPlayerSubsystem` (`GameplayStatics.GetPlayerController` 0)))
  (if bInGame
    (`/Engine/EditorBlueprintResources/StandardMacros.IsValid` (`PlayerController.CheatManager` (`GameplayStatics.GetPlayerController` 0))
      (:`Is Valid`
        (if (`self.bValue`)
          (`EnhancedInputSubsystemInterface.AddMappingContext` _returnvalue "/Game/Design/_GameManagement/Input/IMC_Cheat.IMC_Cheat" 0 (struct))
          (else
            (`EnhancedInputSubsystemInterface.RemoveMappingContext` _returnvalue "/Game/Design/_GameManagement/Input/IMC_Cheat.IMC_Cheat" (struct))))))))