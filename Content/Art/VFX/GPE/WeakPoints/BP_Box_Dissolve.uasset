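; Placeable box actor that defines an oriented dissolve volume for weak point VFX.
; Its construction script writes the Box component's world location, scale and forward, right and up axes into the MPC_Dissolve_WeakPoint material parameter collection.
; Values update only on construction, as BeginPlay is empty and a duplicate copy of the writes in the event graph is unconnected.
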(event `self.ReceiveBeginPlay`)

(fn `UserConstructionScript`
  (bind _box (`self.Box`))
  (`KismetMaterialLibrary.SetVectorParameterValue` "/Game/Art/VFX/Materials/Dissolve/MPC_Dissolve_WeakPoint.MPC_Dissolve_WeakPoint" "Location" (`KismetMathLibrary.Conv_VectorToLinearColor` (`SceneComponent.K2_GetComponentLocation` _box)))
  (`KismetMaterialLibrary.SetVectorParameterValue` "/Game/Art/VFX/Materials/Dissolve/MPC_Dissolve_WeakPoint.MPC_Dissolve_WeakPoint" "Bounds" (`KismetMathLibrary.Conv_VectorToLinearColor` (`SceneComponent.K2_GetComponentScale` _box)))
  (`KismetMaterialLibrary.SetVectorParameterValue` "/Game/Art/VFX/Materials/Dissolve/MPC_Dissolve_WeakPoint.MPC_Dissolve_WeakPoint" "X" (`KismetMathLibrary.Conv_VectorToLinearColor` (`SceneComponent.GetForwardVector` _box)))
  (`KismetMaterialLibrary.SetVectorParameterValue` "/Game/Art/VFX/Materials/Dissolve/MPC_Dissolve_WeakPoint.MPC_Dissolve_WeakPoint" "Y" (`KismetMathLibrary.Conv_VectorToLinearColor` (`SceneComponent.GetRightVector` _box)))
  (`KismetMaterialLibrary.SetVectorParameterValue` "/Game/Art/VFX/Materials/Dissolve/MPC_Dissolve_WeakPoint.MPC_Dissolve_WeakPoint" "Z" (`KismetMathLibrary.Conv_VectorToLinearColor` (`SceneComponent.GetUpVector` _box))))