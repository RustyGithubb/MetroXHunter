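; Base monster Blueprint for the shooting range that reveals its weak points while the player targets it.
; On BeginPlay it caches every BP_WeakPoints child actor found under the capsule component.
; OnSight enables those weak points with the player's look direction and resets a timer.
; Tick advances that timer and disables them once the monster has gone untargeted for over a second.
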(event `self.ReceiveBeginPlay`
  ;[0.3302 0.0085 0 0.33] DEBUG
  (for _array_element (`SceneComponent.GetChildrenComponents` (`self.CapsuleComponent`) true)
    ;[1 1 1 0.33] Get all WeakPoints
    (bind _aschild_actor_component (cast `ChildActorComponent` _array_element))
    (bind _asbp_weak_points (cast `/Game/Design/EyeVisionSystem/BP_WeakPoints` (`ChildActorComponent.ChildActor` _aschild_actor_component)))
    (`KismetArrayLibrary.Array_AddUnique` (`self.WeakPoints`) _asbp_weak_points)))

(event `self.ReceiveTick`
  (params (DeltaSeconds :type "Float (single-precision)"))
  ;[1 1 1 0.33] Check if still Untargeted
  (if (`self.bIsOnSight`)
    (bind _output_get (set `self.OnSightTimer` (+ (`self.OnSightTimer`) DeltaSeconds)))
    (if (> _output_get 1.0)
      ;[1 1 1 0.33] Disable WeakPoints
      (set `self.bIsOnSight` false)
      (for _array_element (`self.WeakPoints`)
        (`/Game/Design/EyeVisionSystem/BP_WeakPoints.DisableWeakPoint` _array_element)))))

(event `OnSight`
  (params (PlayerLookDirection :type "Vector Structure"))
  ;[1 1 1 0.33] Cancel Untargeted Action if the actor is targeted again
  (set `self.bIsOnSight` true)
  (set `self.OnSightTimer` 0.0)
  ;[1 1 1 0.33] Enable WeakPoints
  (for _array_element (`self.WeakPoints`)
    (`/Game/Design/EyeVisionSystem/BP_WeakPoints.EnableWeakPoint` _array_element PlayerLookDirection)))

(fn `UserConstructionScript`)