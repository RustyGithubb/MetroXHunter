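; Setting unit that applies the player's reticle size value to the shooting cursor during gameplay.
; When the setting is applied in game, it finds the first WBP_CursorShoot widget through a class search and caches it while it remains valid.
; It then writes the scaled value as a square image size directly into the CircleCursor brush, doing nothing when applied outside the game.
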(event `self.OnApplySetting`
  (params (bInGame :type Boolean))
  (bind _wbp_cursorshoot (`self.WBP_CursorShoot`))
  (bind _returnvalue (* (`self.Value`) 10.0))
  (if bInGame
    (`/Engine/EditorBlueprintResources/StandardMacros.IsValid` _wbp_cursorshoot
      (:`Is Valid`
        _)
      (:`Is Not Valid`
        (bind _foundwidgets (`WidgetBlueprintLibrary.GetAllWidgetsOfClass` "/Game/Design/Widgets/WBP_CursorShoot.WBP_CursorShoot_C" false))
        (set `self.WBP_CursorShoot` (`|GetArrayItem` _foundwidgets))))
    (setmembers `SlateBrush` :`StructRef` (`Image.Brush` (`/Game/Design/Widgets/WBP_CursorShoot.CircleCursor` _wbp_cursorshoot)) :`ImageSize` (make `DeprecateSlateVector2D` _returnvalue _returnvalue))))