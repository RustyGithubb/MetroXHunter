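; BP_StreetLamp_Cite_B is a street lamp that can be turned on, turned off and flickered.
; BeginPlay caches the bulb's material and the ambient light's intensity.
; Turning off swaps in a fixed bulb material and zeroes the light, while turning on restores both cached values.
; Flicker callbacks expose the ambient light as flickable and swap only the bulb material on start and stop.
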(event `self.ReceiveBeginPlay`
  (`KismetArrayLibrary.Array_Add` (`self.Materials`) (`PrimitiveComponent.GetMaterial` (`self.Bulb`) 0))
  (set `self.AmbiantLightIntensity` (`LightComponentBase.Intensity` (`self.AmbiantLight`))))

(event `TurnOffLights`
  (`self.RemoveEmissiveMaterials`)
  (`LightComponent.SetIntensity` (`self.AmbiantLight`) 0.0))

(event `TurnOnLights`
  (`PrimitiveComponent.SetMaterial` (`self.Bulb`) 0 (`|GetArrayItem` (`self.Materials`)))
  (`LightComponent.SetIntensity` (`self.AmbiantLight`) (`self.AmbiantLightIntensity`)))

(fn `OnFlickLightStart`
  (params (LightData :type "LightData Structure (by ref)"))
  (`PrimitiveComponent.SetMaterial` (`self.Bulb`) 0 "/Game/Design/GPE/Destructible/Lights/MI_BulbTEST.MI_BulbTEST")
  (return))

(fn `OnFlickLightStop`
  (params (LightData :type "LightData Structure (by ref)"))
  (`PrimitiveComponent.SetMaterial` (`self.Bulb`) 0 (`|GetArrayItem` (`self.Materials`)))
  (return))

(fn `OnFlickLightTick`
  (params (DeltaTime :type "Float (single-precision)") (LightData :type "LightData Structure (by ref)"))
  (return))

(fn `OnFlickLightUpdate`
  (params (LightData :type "LightData Structure (by ref)") (IntensityScale :type "Float (single-precision)"))
  (return))

(fn `RemoveEmissiveMaterials`
  (bind _bulb (`self.Bulb`)
    (:`then`
      (`PrimitiveComponent.SetMaterial` _bulb 0 "/Game/Design/GPE/Destructible/Lights/MI_BulbTEST.MI_BulbTEST"))
    (:`else`)))

(fn `RetrieveFlickableLights`
  (returns (ReturnValue :type "Array of LightComponent Object Reference"))
  (return (`|MakeArray` (`self.AmbiantLight`) :!type "LightComponent Object Reference")))

(fn `UserConstructionScript`)