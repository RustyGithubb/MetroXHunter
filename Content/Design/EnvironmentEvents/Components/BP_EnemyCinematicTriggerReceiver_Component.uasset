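; Environment event receiver component that switches a set of enemies into or out of cinematic state when its trigger event plays.
; It loops over valid Enemies and applies the configured InCinematicNewValue through each one's ParasiteAIController.
; With AutoTargetPlayer enabled, it also sets the player character as each controller's enemy.
; The box-enter flag and trigger box passed to the event are unused.
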(fn `OnPlayComponentSpecificEvent`
  (params (FromBoxEnter :type Boolean) (TriggerBox :type "Actor Object Reference"))
  (for _array_element (`self.Enemies`)
    (`/Engine/EditorBlueprintResources/StandardMacros.IsValid` _array_element
      (:`Is Valid`
        (bind _asparasite_aicontroller (cast `ParasiteAIController` (`Pawn.GetController` _array_element)))
        (`ParasiteAIController.SetInCinematic` _asparasite_aicontroller (`self.bInCinematicNewValue`))
        (if (`self.bAutoTargetPlayer`)
          (`ParasiteAIController.SetEnemy` _asparasite_aicontroller (`GameplayStatics.GetPlayerCharacter` 0)))))))