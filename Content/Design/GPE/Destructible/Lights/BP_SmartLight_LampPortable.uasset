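; BP_SmartLight_LampPortable is a destructible portable lamp that goes dark and sparks when its Health component triggers death.
; On death, it destroys every component keyed in the LightIntensityPerComponent map and swaps a Lamp material slot to opaque glass.
; It then plays a transformer deactivation sound at the actor and spawns an enlarged Niagara spark effect at the lamp mesh.
; Construction simply defers to the parent class.
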(event `self.Health.OnDeath`
  (params (DamageContext :type "DamageContext Structure (by ref)"))
  (`self.Explode / Destroy Himself` "/Game/Art/VFX/NS_Electrics/Gun/NS_Lightning_Sparks_Impact.NS_Lightning_Sparks_Impact"))

(fn `Explode / Destroy Himself`
  (params (`Niagara System` :type "NiagaraSystem Object Reference"))
  (bind (_returnvalue_location _returnvalue_rotation) (`KismetMathLibrary.BreakTransform` (`SceneComponent.K2_GetComponentToWorld` (`self.Lamp`))))
  (bind _keys (`BlueprintMapLibrary.Map_Keys` (`self.LightIntensityPerComponent`)))
  (for _array_element _keys
    (`ActorComponent.K2_DestroyComponent` _array_element))
  (`PrimitiveComponent.SetMaterial` (`self.Lamp`) 1 "/Game/Art/VFX/Materials/Glass/M_Glass_Opaque.M_Glass_Opaque")
  ;[1 1 1 0.33] FEEDBACK
  (`GameplayStatics.PlaySoundAtLocation` "/Game/Sounds/Audio/SD/SoundWaves/GPE/Transformator/SW_GPE_Station_Transformator_Desactivation.SW_GPE_Station_Transformator_Desactivation" (`self.K2_GetActorLocation`) (struct) 1.0 1.0 0.0 (`self.Attenuation Settings`) null null null)
  (bind _niagara_system (`local.Niagara System`)
    (:`then`
      (`NiagaraFunctionLibrary.SpawnSystemAtLocation` _niagara_system _returnvalue_location _returnvalue_rotation (5.0 5.0 5.0)))
    (:`else`)))

(fn `UserConstructionScript`
  (`parent.UserConstructionScript`))