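; Door Blueprint, apparently a 3x4 grid, that opens and closes in response to called gameplay events.
; On BeginPlay it binds itself to separate open and close gameplay tags.
; ReceiveEvent matches the incoming tag to OpenGrid or CloseGrid and returns false after either.
; Each sets the Turn flag, toggles the audio component and plays its own actor sequence for the motion.
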(event `self.ReceiveBeginPlay`
  (`/EventDispatcherHub/FunctionLibrary/BPL_EventDispatcherHub.Bind to Single Gameplay Event` (`self.Tag to bind Open`) self)
  (`/EventDispatcherHub/FunctionLibrary/BPL_EventDispatcherHub.Bind to Single Gameplay Event` (`self.Tag to Bind Close`) self))

(fn `Close Grid`
  (set `self.Turn` true)
  (`ActorComponent.ToggleActive` (`self.Audio`))
  (`ActorSequenceComponent.PlaySequence` (`self.ActorSequenceClose`)))

(fn `OpenGrid`
  (set `self.Turn` true)
  ;[0.4281 0.3462 1 0.33] Sound
  (`ActorComponent.ToggleActive` (`self.Audio`))
  ;[1 0 0 0.33] Seqence
  (`ActorSequenceComponent.PlaySequence` (`self.ActorSequence`)))

(fn `ReceiveEvent`
  (params (CalledTag :type "GameplayTag Structure") (CallingObject :type "Object Object Reference (by ref)"))
  (returns (Return :type Boolean))
  (if (== CalledTag (`self.Tag to bind Open`))
    (`self.OpenGrid`)
    (return false)
    (elif (== CalledTag (`self.Tag to Bind Close`))
      (`self.Close Grid`)
      (return false))))

(fn `UserConstructionScript`)