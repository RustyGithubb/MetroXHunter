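; Interactive 2D water surface that drives Niagara ripples and shows lightning arcs when an electrical generator within its box is destroyed.
; With IsWaterDrop enabled, looping timers on BeginPlay pulse drop particles by toggling spawn and kill parameters.
; An overlap check flags the BP_Electrical_Generator_02, and Tick activates the arcs once its health reaches zero.
; A shooting-impact event feeds hit data to Niagara but is marked as a failed test.
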(event `self.ReceiveBeginPlay`
  (if (`self.IsWaterDrop`)
    (`KismetSystemLibrary.K2_SetTimerDelegate` (delegate `SpawnWaterDropParticle`) (/ 60.0 (`self.RateWaterDrop`)) true)
    (`KismetSystemLibrary.K2_SetTimerDelegate` (`|CreateDelegate` :!event `CheckOverlap`) 1.0 true)))

(event `SpawnWaterDropParticle`
  (bind _water_surface (`self.Water_Surface`))
  (`FXSystemComponent.SetBoolParameter` _water_surface "IsKillParticle" false)
  (`FXSystemComponent.SetFloatParameter` _water_surface "SpawnRate" (`self.RateWaterDrop`))
  (`FXSystemComponent.SetVectorParameter` _water_surface "SpawnLocation" (`SceneComponent.K2_GetComponentLocation` _water_surface))
  (`KismetSystemLibrary.DelayUntilNextTick`)
  (`FXSystemComponent.SetBoolParameter` _water_surface "IsKillParticle" true))

(event `CheckOverlap`
  (bind _returnvalue (`GameplayStatics.GetActorOfClass` "/Game/Art/VFX/GPE/Lightnings/BP_Electrical_Generator_02.BP_Electrical_Generator_02_C"))
  (if (`PrimitiveComponent.IsOverlappingActor` (`self.Box`) _returnvalue)
    (set `self.IsOverlapping` true)
    (else
      (set `self.IsOverlapping` false))))

(event `self.ReceiveTick`
  (params (DeltaSeconds :type "Float (single-precision)"))
  (`/Engine/EditorBlueprintResources/StandardMacros.IsValid` (stale `CheckOverlap` _returnvalue)
    (:`Is Valid`
      (if (and (`self.IsOverlapping`) (== (`HealthComponent.CurrentHealth` (`/Game/Art/VFX/GPE/Lightnings/BP_Electrical_Generator_02.Health` (stale `CheckOverlap` _returnvalue))) 0))
        (`/Engine/EditorBlueprintResources/StandardMacros.DoOnce` false
          (:`Completed`
            (`ActorComponent.Activate` (`self.Lightning_Arcs_OnSurface`) false)))))))

(event `/Game/Art/VFX/GPE/Water/BPI_Niagara_Water.GameplayAbilitiesNiagaraWater`
  (params (HitLocation :type "Vector Structure") (HitVelocity :type "Vector Structure") (HitSize :type "Float (double-precision)"))
  (bind _water_surface (`self.Water_Surface`))
  (bind (_returnvalue_x _returnvalue_y _returnvalue_z) (`KismetMathLibrary.BreakVector` (`SceneComponent.K2_GetComponentLocation` _water_surface)))
  ;[0.3823 0 1 0.33] Test to interact with shooting (FAILED)
  (`FXSystemComponent.SetBoolParameter` _water_surface "IsKillParticle" false)
  (`FXSystemComponent.SetVectorParameter` _water_surface "SpawnLocation" (`KismetMathLibrary.MakeVector` (.x HitLocation) (.y HitLocation) _returnvalue_z))
  (`FXSystemComponent.SetVectorParameter` _water_surface "HitVelocity" (`KismetMathLibrary.MakeVector` (.x HitVelocity) (.y HitVelocity)))
  (`FXSystemComponent.SetFloatParameter` _water_surface "HitSize" HitSize)
  (`FXSystemComponent.SetFloatParameter` _water_surface "SpawnRate" 20.0)
  (`KismetSystemLibrary.RetriggerableDelay` 0.2)
  (`FXSystemComponent.SetBoolParameter` _water_surface "IsKillParticle" true)
  (`FXSystemComponent.SetFloatParameter` _water_surface "SpawnRate" 0.0))

(fn `UserConstructionScript`)