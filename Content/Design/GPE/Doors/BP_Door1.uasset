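; BP_Door1 is a swinging door that rotates open around its yaw axis.
; SetDoorOpened plays a timeline that turns the door from its starting yaw toward a target whose direction the construction script sets from FlipRotation, then marks it opened and freezes interaction.
; Box overlaps are passed to OnDoorHit, an editor event resets the yaw to zero, and SetDoorOpened has no closing branch.
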(event `self.ReceiveBeginPlay`
  (bind (_relativerotation_roll _relativerotation_pitch _relativerotation_yaw) (`KismetMathLibrary.BreakRotator` (`SceneComponent.RelativeRotation` (`self.Door`))))
  (set `self.StartYawRotation` _relativerotation_yaw))

(event `self.Box.OnComponentBeginOverlap`
  (params (OverlappedComponent :type "PrimitiveComponent Object Reference") (OtherActor :type "Actor Object Reference") (OtherComp :type "PrimitiveComponent Object Reference") (OtherBodyIndex :type Integer) (bFromSweep :type Boolean) (SweepResult :type "HitResult Structure (by ref)"))
  (`self.OnDoorHit` OtherActor))

(event `self.SetDoorOpened`
  (params (bShouldOpen :type Boolean))
  (if bShouldOpen
    (bind (_direction _rotation) (`Timeline|OpenDoor` :!via `PlayFromStart`)
      (:`Update`
        (`SceneComponent.K2_SetRelativeRotation` (`self.Door`) (`KismetMathLibrary.MakeRotator` 0.0 0.0 (+ (* _rotation (`self.TargetRotation`)) (`self.StartYawRotation`))) false false))
      (:`Finished`
        (set `self.bIsOpened` true)
        (`self.SetInteractionFreezed` true)))))

(event `self.CloseDoorEditor`
  (`SceneComponent.K2_SetRelativeRotation` (`self.Door`) (`KismetMathLibrary.MakeRotator` 0.0) false false))

(fn `UserConstructionScript`
  (if (`self.bFlipRotation`)
    (set `self.TargetRotation` 150.0)
    (else
      (set `self.TargetRotation` -150.0))))