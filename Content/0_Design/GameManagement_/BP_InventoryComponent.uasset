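; BP_InventoryComponent tracks the player's default ammo and healing syringe segments, starting and capping both from InventoryValues.
; AddToInventory adds either item by type, using CheckForOverflow to clamp at the maximum and return the excess.
; Helpers clear or max out each resource and check whether the syringe is full.
; Changes call visual updates: ammo refreshes the HUD count, while the syringe update is an empty stub.
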(event `self.ReceiveBeginPlay`
  (`|ExecutionSequence`
    (:`then_0`
      (set `self.CurrentDefaultAmmoAmount` (`/Game/0_Design/GameManagement_/PDA_InventoryValues.StartingDefaultAmmoAmount` (`self.InventoryValues`)))
      (`self.VisuallyUpdateAmmoAmount`))
    (:`then_1`
      (set `self.CurrentSyringeSegments` (`/Game/0_Design/GameManagement_/PDA_InventoryValues.StartingSyringeCapacity` (`self.InventoryValues`)))
      (`self.VisuallyUpdateSyringe`))))

(fn `AddToInventory`
  (params (`Object Type` :type "/Game/3_GPE/PickupLoot/E_PickupType Enum" :default "NewEnumerator0") (Amount :type Integer))
  (returns (Overflow :type Integer))
  (locals (OverflowAmount :type Integer))
  (`|ExecutionSequence`
    (:`then_0`
      (switch `/Game/3_GPE/PickupLoot/E_PickupType` `Object Type`
        (:`NewEnumerator0`
          (bind (_overflow _finalamount) (`self.CheckForOverflow` (`local.Amount`) (`self.CurrentDefaultAmmoAmount`) (`/Game/0_Design/GameManagement_/PDA_InventoryValues.MaxDefaultAmmoAmount` (`self.InventoryValues`))))
          (set `local.OverflowAmount` _overflow)
          (set `self.CurrentDefaultAmmoAmount` _finalamount)
          (`self.VisuallyUpdateAmmoAmount`))
        (:`NewEnumerator1`
          (bind (_overflow_2 _finalamount_2) (`self.CheckForOverflow` (`local.Amount`) (`self.CurrentSyringeSegments`) (`/Game/0_Design/GameManagement_/PDA_InventoryValues.MaxSyringeCapacity` (`self.InventoryValues`))))
          (set `local.OverflowAmount` _overflow_2)
          (set `self.CurrentSyringeSegments` _finalamount_2)
          (`self.VisuallyUpdateSyringe`))))
    (:`then_1`
      ;[1 1 1 0.33] Return Overflow
      (return (`local.OverflowAmount`)))))

(fn `CheckForOverflow`
  (params (AmountToAdd :type Integer) (CurrentAmount :type Integer) (MaxAmount :type Integer))
  (returns (Overflow :type Integer) (FinalAmount :type Integer))
  (locals (NewAmount :type Integer) (OverflowAmount :type Integer))
  ;[1 1 1 0.33] New Amount
  (bind _output_get (set `local.NewAmount` (+ AmountToAdd CurrentAmount)))
  ;[1 1 1 0.33] OverFlow Amount
  (bind _output_get_2 (set `local.OverflowAmount` (- _output_get MaxAmount)))
  (if (> _output_get_2 0)
    (set `local.NewAmount` (`local.MaxAmount`))
    (else
      (set `local.OverflowAmount` 0)))
  (return (`local.OverflowAmount`) (`local.NewAmount`)))

(fn `ClearDefaultAmmo`
  (set `self.CurrentDefaultAmmoAmount` 0)
  (`self.VisuallyUpdateAmmoAmount`))

(fn `ClearSyringeSegments`
  (set `self.CurrentSyringeSegments` 0)
  (`self.VisuallyUpdateSyringe`))

(fn `FullyFillHealingSyringe`
  (set `self.CurrentSyringeSegments` (`/Game/0_Design/GameManagement_/PDA_InventoryValues.MaxSyringeCapacity` (`self.InventoryValues`)))
  (`self.VisuallyUpdateSyringe`))

(fn `GiveMaxDefaultAmmo`
  (set `self.CurrentDefaultAmmoAmount` (`/Game/0_Design/GameManagement_/PDA_InventoryValues.MaxDefaultAmmoAmount` (`self.InventoryValues`)))
  (`self.VisuallyUpdateAmmoAmount`))

(fn `IsSyringeFull`
  (returns (NewParam :type Boolean))
  (return (== (`self.CurrentSyringeSegments`) (`/Game/0_Design/GameManagement_/PDA_InventoryValues.MaxSyringeCapacity` (`self.InventoryValues`)))))

(fn `VisuallyUpdateAmmoAmount`
  (message `/Game/0_Design/GameManagement_/BPI_HUD.UpdateAmmoCount` (`PlayerController.GetHUD` (`GameplayStatics.GetPlayerController` 0))))

(fn `VisuallyUpdateSyringe`)