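; Trigger receiver component for environment events that sets event flags on the player when its event plays.
; On BeginPlay it caches the BP_EventFlagsComponent from player pawn 0.
; OnPlayComponentSpecificEvent writes every name and value pair in the TagsToSetAndValues map to that component through SetFlagValue, ignoring the FromBoxEnter argument.
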(event `self.ReceiveBeginPlay`
  (set `self.PlayerFlagComponent` (`Actor.GetComponentByClass` (`GameplayStatics.GetPlayerPawn` 0) "/Game/0_Design/EnvironmentEvents/BP_EventFlagsComponent.BP_EventFlagsComponent_C")))

(fn `OnPlayComponentSpecificEvent`
  (params (FromBoxEnter :type Boolean))
  (bind _tagstosetandvalues (`self.TagsToSetAndValues`))
  (bind _keys (`BlueprintMapLibrary.Map_Keys` _tagstosetandvalues))
  (bind _values (`BlueprintMapLibrary.Map_Values` _tagstosetandvalues))
  (for (_array_element _array_index) _keys
    (`/Game/0_Design/EnvironmentEvents/BP_EventFlagsComponent.SetFlagValue` (`self.PlayerFlagComponent`) _array_element (`|GetArrayItem` _values _array_index))))