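; Developer player controller that toggles an on-screen cheat menu with the Tab debug key.
; The key press requires an MXHCheatManager, then either creates WBP_CheatMenu and fills it from that manager, or removes and clears the open menu.
; Input mode switches to game-and-UI while the menu is shown and back to game-only when it closes.
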(event EventBeginPlay)

(event EventTick
  (params (DeltaSeconds :type Float%20%28single-precision%29)))

(event Input|KeyboardEvents|DebugKeyTab
  (params (Key :type Key%20Structure :default "None") (ActionValue :type Input%20Action%20Value%20Structure))
  (bind _self self)
  (:Pressed
    (bind _asmxhcheat_manager (Utilities|Casting|CastToMXHCheatManager (Variables|Default|GetCheatManager)))
    (bind _cheat_menu (Variables|Default|GetCheat%20Menu)
      (:then
        (Widget|RemovefromParent _cheat_menu)
        (Variables|Default|SetCheat%20Menu 0)
        (Input|SetInputModeGameOnly _self false))
      (:else
        (bind _returnvalue (UserInterface|CreateWidget "/Game/Cheats/WBP_CheatMenu.WBP_CheatMenu_C" self))
        (bind _output_get (Variables|Default|SetCheat%20Menu _returnvalue))
        (UserInterface|Viewport|AddtoViewport _output_get 0)
        (Default|PopulateCheats _output_get _asmxhcheat_manager)
        (Input|SetInputModeGameandUI _self 0 "DoNotLock" false false)))))

(fn ConstructionScript)