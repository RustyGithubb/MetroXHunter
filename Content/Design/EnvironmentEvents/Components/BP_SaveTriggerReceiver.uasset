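; BP_SaveTriggerReceiver is an environment event receiver component that saves the level as a checkpoint when its event plays.
; It first reads the checkpoint setting from the Metro settings subsystem, then confirms through the game mode that the world is fully loaded.
; When both checks pass, it calls SaveLevel on the game instance, regardless of which trigger box fired or whether it was a box enter.
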(fn `OnPlayComponentSpecificEvent`
  (params (FromBoxEnter :type Boolean) (TriggerBox :type "Actor Object Reference"))
  (bind _returnvalue (`MetroSettingsSubsystem.FindSettingOfClass` (subsystem `MetroSettingsSubsystem`) "/Game/Design/Settings/Units/Gameplay/BP_SettingUnit_Checkpoint.BP_SettingUnit_Checkpoint_C"))
  (if (`MetroSettingUnitBool.bValue` _returnvalue)
    (bind _asmetro_game_mode (cast `MetroGameMode` (`GameplayStatics.GetGameMode`)))
    (if (`MetroGameMode.IsWorldFullyLoaded` _asmetro_game_mode)
      (bind _asmetro_game_instance (cast `MetroGameInstance` (`GameplayStatics.GetGameInstance`)))
      (`MetroGameInstance.SaveLevel` _asmetro_game_instance))))