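; Trigger receiver component that plays cinematic level sequences when its component-specific trigger event fires.
; It starts its own sequence and the LevelSequenceHandler's, with optional player hiding, input freezing, view blend to the handler's CineCamera and player relocation.
; The finish handler signals sequence end, prints a debug string and restores visibility and input, but does not blend the view back.
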(fn `OnPlayComponentSpecificEvent`
  (params (FromBoxEnter :type Boolean) (TriggerBox :type "Actor Object Reference"))
  (add `MovieSceneSequencePlayer.OnFinished` (`LevelSequenceActor.SequencePlayer` (`LevelSequencerHandler.LevelSequenceActor` (`self.LevelSequenceHandler`))) (`|CreateDelegate` :!event `OnSequenceFinished`))
  (`MovieSceneSequencePlayer.Play` (`LevelSequenceActor.SequencePlayer` (`self.LevelSequence`)))
  (if (`self.ShouldHideChara`)
    (`Actor.SetActorHiddenInGame` (`GameplayStatics.GetPlayerCharacter` 0) true))
  (if (`self.ShouldFreezeInputs`)
    (`Actor.DisableInput` (`GameplayStatics.GetPlayerController` 0) null)
    (`Actor.DisableInput` (`GameplayStatics.GetPlayerCharacter` 0) null))
  (if (`self.ShouldBlend`)
    (`PlayerController.SetViewTargetWithBlend` (`GameplayStatics.GetPlayerController` 0) (`LevelSequencerHandler.CineCamera` (`self.LevelSequenceHandler`)) (`self.Blend Time`) (`self.Blend Func`) (`self.Blend Exp`) false))
  (`MovieSceneSequencePlayer.Play` (`LevelSequenceActor.SequencePlayer` (`LevelSequencerHandler.LevelSequenceActor` (`self.LevelSequenceHandler`))))
  (if (`self.Should change position`)
    (`Actor.K2_SetActorLocation` (`GameplayStatics.GetPlayerCharacter` 0) (`self.New Player Location`) false false)))

(fn `OnSequenceFinished`
  (`self.OnSequenceEnd`)
  (`KismetSystemLibrary.PrintString` "Hello")
  (if (`self.ShouldHideChara`)
    (`Actor.SetActorHiddenInGame` (`GameplayStatics.GetPlayerCharacter` 0) false))
  (if (`self.ShouldFreezeInputs`)
    (`Actor.EnableInput` (`GameplayStatics.GetPlayerController` 0) null)
    (`Actor.EnableInput` (`GameplayStatics.GetPlayerCharacter` 0) null)))