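; BP_Grid is a configurable grid-and-door piece for the metro tunnels playground.
; The construction script uses Hole to raise and squash the Door, and Turn to tilt the Grid.
; BeginPlay reapplies the Hole scale but raises the Door in both cases, unlike the construction script.
; Two helper functions, not called here, toggle visibility and navigation relevance on given meshes and lights, plus mesh collision.
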(event `self.ReceiveBeginPlay`
  (bind _door (`self.Door`))
  (bind _door_2 (`self.Door`))
  (if (`self.Hole`)
    (`SceneComponent.K2_SetRelativeLocation` _door_2 (100.0 0.0 300.0) false false)
    (`SceneComponent.SetRelativeScale3D` _door_2 (1.0 1.0 0.4))
    (else
      (`SceneComponent.K2_SetRelativeLocation` _door (100.0 0.0 300.0) false false)
      (`SceneComponent.SetRelativeScale3D` _door (1.0 1.0 1.0)))))

(fn `DisableCollisionAndVisibility`
  (params (`Static Meshes` :type "Array of StaticMeshComponent Object Reference") (Lights :type "Array of LightComponent Object Reference"))
  ;[1 0.5264 0.4766 0.33] DisableSM
  (for _array_element `Static Meshes`
    (`SceneComponent.SetHiddenInGame` _array_element true false)
    (`SceneComponent.SetVisibility` _array_element false false)
    (`PrimitiveComponent.SetCollisionEnabled` _array_element "NoCollision")
    (`UtilityLibrary.SetActorComponentCanEverAffectNavigation` _array_element))
  ;[1 0.8982 0.4238 0.33] DisableLights
  (for _array_element_2 Lights
    (`SceneComponent.SetHiddenInGame` _array_element_2 true false)
    (`SceneComponent.SetVisibility` _array_element_2 false false)
    (`UtilityLibrary.SetActorComponentCanEverAffectNavigation` _array_element_2))
  (return))

(fn `EnableCollisionAndVisibility`
  (params (`Static Meshes` :type "Array of StaticMeshComponent Object Reference") (Lights :type "Array of LightComponent Object Reference"))
  ;[1 0.5264 0.4766 0.33] EnableSM
  (for _array_element `Static Meshes`
    (`SceneComponent.SetHiddenInGame` _array_element false false)
    (`SceneComponent.SetVisibility` _array_element true false)
    (`PrimitiveComponent.SetCollisionEnabled` _array_element "QueryAndPhysics")
    (`UtilityLibrary.SetActorComponentCanEverAffectNavigation` _array_element true))
  ;[1 0.8982 0.4238 0.33] EnableLights
  (for _array_element_2 Lights
    (`SceneComponent.SetHiddenInGame` _array_element_2 false false)
    (`SceneComponent.SetVisibility` _array_element_2 true false)
    (`UtilityLibrary.SetActorComponentCanEverAffectNavigation` _array_element_2 true))
  (return))

(fn `UserConstructionScript`
  (bind _door (`self.Door`))
  (bind _door_2 (`self.Door`))
  (if (`self.Hole`)
    (`SceneComponent.K2_SetRelativeLocation` _door_2 (100.0 0.0 300.0) false false)
    (`SceneComponent.SetRelativeScale3D` _door_2 (1.0 1.0 0.4))
    (else
      (`SceneComponent.K2_SetRelativeLocation` _door (100.0 0.0 0.0) false false)
      (`SceneComponent.SetRelativeScale3D` _door (1.0 1.0 1.0))))
  (if (`self.Turn`)
    (`SceneComponent.K2_SetRelativeRotation` (`self.Grid`) (struct :`Yaw` -70.0) false false)
    (else
      (`SceneComponent.K2_SetRelativeRotation` (`self.Grid`) (struct) false false))))