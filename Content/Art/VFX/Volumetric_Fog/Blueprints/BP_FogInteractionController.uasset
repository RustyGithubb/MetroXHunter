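; Controller actor that drives 2D interaction for volumetric fog around the player character or its own location.
; On BeginPlay it clears the fog render target and, if interaction is enabled, pushes distortion and trail settings to MPC_FogVolumetrics and spawns a top-down scene capture.
; Tick snaps the capture's XY to a 512-texel grid to follow the target, publishes RTPosition to the collection, and moves an optional debug zone.
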(event EventBeginPlay
  (CallFunction|InitializeCapture))

(event EventTick
  (params (DeltaSeconds :type Float%20%28single-precision%29))
  (if (Variables|Default|GetCapturePlayer)
    (Variables|Default|SetLocation (Transformation|GetActorLocation (Game|GetPlayerCharacter 0)))
    (else
      (Variables|Default|SetLocation (Transformation|GetActorLocation))))
  (Transformation|SetWorldLocation (Variables|Default|GetDefaultSceneRoot) (Math|Vector|MakeVector 0.0 0.0 (+ (.z (Variables|Default|GetLocation)) 1.2e+03)) false false)
  (Transformation|AddWorldOffset (Variables|Default|GetSceneCapture) (Math|Vector|MakeVector (.x (- (|(((vector((floor((X/PixelWorldSize))),(floor((Y/PixelWorldSize))),0))+0.500000)*PixelWorldSize) (* (Variables|/Script/Engine.SceneCaptureComponent2D|GetOrthoWidth (Variables|Default|GetSceneCapture)) (/ 1.0 512.0)) (.x (Variables|Default|GetLocation)) (.y (Variables|Default|GetLocation))) (Transformation|GetWorldLocation (Variables|Default|GetSceneCapture)))) (.y (- (|(((vector((floor((X/PixelWorldSize))),(floor((Y/PixelWorldSize))),0))+0.500000)*PixelWorldSize) (* (Variables|/Script/Engine.SceneCaptureComponent2D|GetOrthoWidth (Variables|Default|GetSceneCapture)) (/ 1.0 512.0)) (.x (Variables|Default|GetLocation)) (.y (Variables|Default|GetLocation))) (Transformation|GetWorldLocation (Variables|Default|GetSceneCapture)))) 0.0) false false)
  (Rendering|Material|SetVectorParameterValue "/Game/Art/VFX/Volumetric_Fog/Material/MPC_FogVolumetrics.MPC_FogVolumetrics" "RTPosition" (Utilities|Struct|MakeLinearColor (.x (Variables|Default|GetLocation)) (.y (Variables|Default|GetLocation)) (.z (Variables|Default|GetLocation)) 1.0) :!class /Script/Engine.KismetMaterialLibrary)
  (if (Variables|Default|GetDebugInteractionZoneEnable)
    (Transformation|SetWorldLocation (Variables|Default|GetDebug) (- (Transformation|GetWorldLocation (Variables|Default|GetSceneCapture)) "0.000000,0.000000,1150.000000") false false)))

(fn ConstructionScript
  (Rendering|SetVisibility (Variables|Default|GetDebug) (Variables|Default|GetDebugInteractionZoneEnable) false))

(fn InitializeCapture
  (Rendering|ClearRenderTarget2D "/Game/Art/VFX/Volumetric_Fog/Textures/T_Fog_RT.T_Fog_RT")
  (if (Variables|Default|GetInteraction2DEnable)
    (Rendering|Material|SetVectorParameterValue "/Game/Art/VFX/Volumetric_Fog/Material/MPC_FogVolumetrics.MPC_FogVolumetrics" "RTDistortionAmount" (Utilities|Struct|MakeLinearColor (Variables|Default|GetRTDistortionUVScale) (Variables|Default|GetRTDistortionAmount) (Variables|Default|GetRTDistortionContrast) 0.0) :!class /Script/Engine.KismetMaterialLibrary)
    (Rendering|Material|SetVectorParameterValue "/Game/Art/VFX/Volumetric_Fog/Material/MPC_FogVolumetrics.MPC_FogVolumetrics" "TrailVisibility" (Utilities|Struct|MakeLinearColor (Variables|Default|GetTrailVisibilityObjects) (Variables|Default|GetTrailVisibilityPlayer) 0.0 0.0) :!class /Script/Engine.KismetMaterialLibrary)
    (if (Variables|Default|GetCapturePlayer)
      (Utilities|IsValid (Game|GetPlayerCharacter 0)
        (:Is%20Valid
          _)))
    (bind _returnvalue (AddComponent|AddSceneCaptureComponent2D false (Math|Transform|MakeTransform (Math|Vector|SelectVector (.Location (CallFunction|PlayerTransform 0.0)) (Transformation|GetActorLocation) (Variables|Default|GetCapturePlayer)) "-90.000000,90.000000,0.000000" "1.000000,1.000000,1.000000")))
    (Variables|Default|SetSceneCapture _returnvalue)
    (Actor|Tick|SetActorTickEnabled true)))

(fn PlayerTransform
  (params (ForwardDistance :type Float%20%28double-precision%29))
  (bind _returnvalue (Game|GetPlayerCharacter 0))
  (bind _returnvalue_2 (Transformation|GetActorLocation _returnvalue))
  (bind _returnvalue_3 (Transformation|GetActorForwardVector _returnvalue))
  (Utilities|IsValid _returnvalue
    (:Is%20Valid
      (return _returnvalue_2 (+ _returnvalue_2 (* _returnvalue_3 ForwardDistance)) _returnvalue_3))))

(fn MakeVector4
  (params (Start :type Vector) (Size :type Float%20%28double-precision%29))
  (bind (_x _y _z) (Math|Vector|BreakVector Start))
  (return (Math|Color|MakeColor _x _y _z Size)))