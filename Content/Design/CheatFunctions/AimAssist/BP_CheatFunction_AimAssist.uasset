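; Cheat function that switches the player pawn's aim assist component on or off based on its selected index.
; After a one-tick delayed init, it caches that component plus the Difficulty and AimAssist Debug cheat functions from the CheatManager.
; Disabling also fires the debug cheat if togglable and resets the index.
; Both options run a check that moves the Difficulty cheat to another index when its current one conflicts with the new state.
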(event `self.OnInit`
  (`KismetSystemLibrary.DelayUntilNextTick`)
  (`self.GetReferences`))

(event `self.OnCheat`
  (bind _index (`MetroCheatSelectionFunction.Index` (`self.DifficultyCheatFunction`)))
  (switch `int` (`self.Index`)
    (:`0`
      (`self.DisableAimAssist`)
      (if (!= _index 2)
        (set `MetroCheatSelectionFunction.Index` 3 (`self.DifficultyCheatFunction`) :!label _label)))
    (:`1`
      (set `/AdvancedAimAssist/Blueprints/Components/AAA_BP_AimAssistComponent.bIsAimAssistEnable` true (`self.AimAssistComponent`))
      (if (not (< _index 2))
        (goto _label)))))

(fn `DisableAimAssist`
  (bind _aimassistdebugcheatfunction (`self.AimAssistDebugCheatFunction`))
  (`|ExecutionSequence`
    (:`then_0`
      (if (`MetroCheatFunction.bIsTogglable` _aimassistdebugcheatfunction)
        (`self.Cheat` :`self` _aimassistdebugcheatfunction)))
    (:`then_1`
      (set `/AdvancedAimAssist/Blueprints/Components/AAA_BP_AimAssistComponent.bIsAimAssistEnable` false (`self.AimAssistComponent`))
      (if (!= (`self.Index`) 0)
        (set `self.Index` 0)))))

(fn `GetReferences`
  (bind _returnvalue (`Controller.K2_GetPawn` (`CheatManager.GetPlayerController` (`self.CheatManager`))))
  (`/Engine/EditorBlueprintResources/StandardMacros.IsValid` _returnvalue
    (:`Is Valid`
      (set `self.AimAssistComponent` (`Actor.GetComponentByClass` _returnvalue "/AdvancedAimAssist/Blueprints/Components/AAA_BP_AimAssistComponent.AAA_BP_AimAssistComponent_C"))
      (`|ExecutionSequence`
        (:`then_0`
          (bind _returnvalue_2 (`MetroCheatManager.FindCheatFunctionOfClass` (`self.CheatManager`) "/Game/Design/CheatFunctions/BP_CheatFunction_Difficulty.BP_CheatFunction_Difficulty_C"))
          (set `self.DifficultyCheatFunction` _returnvalue_2))
        (:`then_1`
          (bind _returnvalue_3 (`MetroCheatManager.FindCheatFunctionOfClass` (`self.CheatManager`) "/Game/Design/CheatFunctions/AimAssist/BP_CheatFunction_AimAssist_Debug.BP_CheatFunction_AimAssist_Debug_C"))
          (set `self.AimAssistDebugCheatFunction` _returnvalue_3))))))