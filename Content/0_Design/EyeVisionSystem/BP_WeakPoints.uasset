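; Weak point actor for the eye vision system: hidden by default, it appears only when enabled and seen from the right direction.
; While enabled, each Tick compares the player's look direction to its forward vector by dot product, toggling visibility and collision.
; Options allow two-sided or constant visibility.
; On death it turns black and scales down via timeline, then resets its life and scales back up after a respawn delay.
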(event `self.ReceiveBeginPlay`
  ;[0.4802 0 0.01596 0.33] BEGINPLAY
  (set `self.InitialeScale` (`self.GetActorScale3D` self))
  (`self.SetActorHiddenInGame` true))

(event `self.LifeComponent.OnDeath`
  ;[1 1 1 0.33] OnDeath
  (`PrimitiveComponent.SetMaterial` (`self.Cube`) 0 "/Game/9_ShootingRange/Materials/MI_FlatColor_Black.MI_FlatColor_Black")
  (`self.ScaleDownTimeline`)
  (`KismetSystemLibrary.Delay` (`self.RespawnDelay`))
  (`/Game/0_Design/LifeSystem/BP_LifeComponent.ResetLife` (`self.LifeComponent`))
  (`self.ScaleUpTimeline`)
  (`PrimitiveComponent.SetMaterial` (`self.Cube`) 0 "/Engine/BasicShapes/BasicShapeMaterial.BasicShapeMaterial"))

(event `self.ReceiveTick`
  (params (DeltaSeconds :type "Float (single-precision)"))
  ;[0.4802 0 0.01596 0.33] TICK
  (if (`self.IsEnable`)
    (`self.CheckVisionDetection`)))

(event `EnableWeakPoint`
  (params (LookDirection :type "Vector Structure"))
  ;[1 1 1 0.33] ENABLE WEAKPOINT
  (set `self.IsEnable` true)
  (set `self.PlayerLook Direction` LookDirection))

(event `DisableWeakPoint`
  ;[1 1 1 0.33] DISABLE WEAKPOINT
  (set `self.IsEnable` false)
  (`self.SetActorHiddenInGame` true))

(event `ScaleUpTimeline`
  (bind (_direction _scale) (`Timeline|ScaleMultiplier` :!via `PlayFromStart` :!label _label)
    (:`Update`
      (`self.SetActorScale3D` self (* (`self.InitialeScale`) _scale)))))

(event `ScaleDownTimeline`
  (goto _label :!via `ReverseFromEnd`))

(fn `CheckVisionDetection`
  (if (not (`self.IsAlwaysVisible?`))
    (if (not (`self.IsVisibleFromBothSide?`))
      (if (`self.DotProduct` (`self.VisibleAngle`))
        (`self.SetActorHiddenInGame` false :!label _label)
        (`PrimitiveComponent.SetCollisionEnabled` (`self.Cube`) "QueryOnly")
        (else
          (`self.SetActorHiddenInGame` true :!label _label_2)
          (`PrimitiveComponent.SetCollisionEnabled` (`self.Cube`) "NoCollision")))
      (elif (or (`self.DotProduct` (`self.VisibleAngle`)) (`self.DotProduct` (* (`self.VisibleAngle`) -1.0) true))
        (goto _label)
        (else
          (goto _label_2))))
    (elif (`self.bHidden`)
      (`self.SetActorHiddenInGame` false))))

(fn `DotProduct`
  (params (VisionAngle :type "Float (double-precision)") (Switch :type Boolean))
  (returns (ReturnValue :type Boolean))
  (bind _returnvalue (`KismetMathLibrary.Dot_VectorVector` (`self.PlayerLook Direction`) (`self.GetActorForwardVector`)))
  (if (not Switch)
    (return (< _returnvalue VisionAngle))
    (else
      (return (> _returnvalue VisionAngle)))))

(fn `UserConstructionScript`)