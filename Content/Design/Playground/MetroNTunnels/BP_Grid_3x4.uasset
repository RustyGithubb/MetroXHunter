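; Metro tunnel grid door that opens and closes on gameplay tags, snapping the door's yaw by FinalRotation with sounds and a green or red lamp and light.
; Turn previews the open pose in the construction script.
; BeginPlay binds both tags; ReceiveEvent runs OpenGrid or CloseGrid, then saves IsConsummed as true in either case.
; On load, a consumed state calls OpenGrid, so a closed grid also reloads open.
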(event `self.ReceiveBeginPlay`
  (`/EventDispatcherHub/FunctionLibrary/BPL_EventDispatcherHub.Bind to Single Gameplay Event` (`self.Tag to bind Open`) self)
  (`/EventDispatcherHub/FunctionLibrary/BPL_EventDispatcherHub.Bind to Single Gameplay Event` (`self.Tag to Bind Close`) self))

(event `self.SaveLoad.OnLoadActor`
  ;[0 1 0.05748 0.33] ON LOAD
  (bind _value (`StructUtilsFunctionLibrary.GetInstancedStructValue` (`SaveLoadComponent.SavedData` (`self.SaveLoad`)))
    (:`Valid`
      (if (`.bIsConsummed` (break `InteractableSavedData` _value))
        (`self.OpenGrid`)))))

(fn `CloseGrid`
  (bind _pointlight (`self.PointLight`))
  (bind _sm_grid_staff_door (`self.SM_Grid_Staff_Door`))
  (bind (_relativerotation_roll _relativerotation_pitch _relativerotation_yaw) (`KismetMathLibrary.BreakRotator` (`SceneComponent.RelativeRotation` _sm_grid_staff_door)))
  (set `self.Turn` true)
  (`ActorComponent.ToggleActive` (`self.Audio`))
  (`GameplayStatics.PlaySoundAtLocation` "/Game/Sounds/Audio/SFX/SFX_GPE/SFX_Grid/SC_GridClosing.SC_GridClosing" (+ (`SceneComponent.RelativeLocation` (`self.SM_Grid_Staff_Door`)) (0.0 0.0 38.0)) (struct) 1.0 1.0 0.0 null null null null)
  (`LightComponent.SetLightColor` _pointlight (struct :`R` 1.0 :`A` 1.0) true)
  (`LightComponent.SetLightFunctionMaterial` _pointlight "/Game/Art/LevelPrototyping/Lights/LightFunctions/LF_FlickeringNeonBright_Red.LF_FlickeringNeonBright_Red")
  (`PrimitiveComponent.SetMaterial` (`self.Lamp`) 2 "/Game/Art/LevelPrototyping/Lights/LightFunctions/LF_FlickeringNeonBright_Red.LF_FlickeringNeonBright_Red")
  (`SceneComponent.K2_SetRelativeRotation` _sm_grid_staff_door (`KismetMathLibrary.MakeRotator` _relativerotation_roll _relativerotation_pitch (- _relativerotation_yaw (`self.FinalRotation`))) false false))

(fn `DisableCollisionAndVisibility`
  (params (`Static Meshes` :type "Array of StaticMeshComponent Object Reference") (Lights :type "Array of LightComponent Object Reference"))
  ;[1 0.5264 0.4766 0.33] DisableSM
  (for _array_element `Static Meshes`
    (`SceneComponent.SetHiddenInGame` _array_element true false)
    (`SceneComponent.SetVisibility` _array_element false false)
    (`PrimitiveComponent.SetCollisionEnabled` _array_element "NoCollision")
    (`UtilityLibrary.SetActorComponentCanEverAffectNavigation` _array_element))
  ;[1 0.8982 0.4238 0.33] DisableLights
  (for _array_element_2 Lights
    (`SceneComponent.SetHiddenInGame` _array_element_2 true false)
    (`SceneComponent.SetVisibility` _array_element_2 false false)
    (`UtilityLibrary.SetActorComponentCanEverAffectNavigation` _array_element_2))
  (return))

(fn `EnableCollisionAndVisibility`
  (params (`Static Meshes` :type "Array of StaticMeshComponent Object Reference") (Lights :type "Array of LightComponent Object Reference"))
  ;[1 0.5264 0.4766 0.33] EnableSM
  (for _array_element `Static Meshes`
    (`SceneComponent.SetHiddenInGame` _array_element false false)
    (`SceneComponent.SetVisibility` _array_element true false)
    (`PrimitiveComponent.SetCollisionEnabled` _array_element "QueryAndPhysics")
    (`UtilityLibrary.SetActorComponentCanEverAffectNavigation` _array_element true))
  ;[1 0.8982 0.4238 0.33] EnableLights
  (for _array_element_2 Lights
    (`SceneComponent.SetHiddenInGame` _array_element_2 false false)
    (`SceneComponent.SetVisibility` _array_element_2 true false)
    (`UtilityLibrary.SetActorComponentCanEverAffectNavigation` _array_element_2 true))
  (return))

(fn `OpenGrid`
  (bind _pointlight (`self.PointLight`))
  (bind _returnvalue (`SceneComponent.K2_GetComponentLocation` (`self.SM_Grid_Staff_Door`)))
  (set `self.Turn` true)
  ;[0.4281 0.3462 1 0.33] Sound
  (`ActorComponent.ToggleActive` (`self.Audio`))
  (`GameplayStatics.PlaySoundAtLocation` "/Game/Sounds/Audio/SFX/SFX_GPE/SFX_Grid/SC_GridUnlock.SC_GridUnlock" _returnvalue (struct) 1.0 1.0 0.0 null null null null)
  (`GameplayStatics.PlaySoundAtLocation` "/Game/Sounds/Audio/SFX/SFX_GPE/SFX_Grid/SC_GridOpening.SC_GridOpening" _returnvalue (struct) 1.0 1.0 0.0 null null null null)
  (`LightComponent.SetLightColor` _pointlight (struct :`R` 0.119778 :`G` 1.0 :`A` 1.0) true)
  (`LightComponent.SetLightFunctionMaterial` _pointlight null)
  (`PrimitiveComponent.SetMaterial` (`self.Lamp`) 2 "/Game/Art/LevelPrototyping/Lights/Emissives/M_NeonGreen.M_NeonGreen")
  (`SceneComponent.K2_SetRelativeRotation` (`self.SM_Grid_Staff_Door`) (`KismetMathLibrary.MakeRotator` 0.0 0.0 (`self.FinalRotation`)) false false))

(fn `ReceiveEvent`
  (params (CalledTag :type "GameplayTag Structure") (CallingObject :type "Object Object Reference (by ref)"))
  (returns (Return :type Boolean))
  (bind _saveddata (`SaveLoadComponent.SavedData` (`self.SaveLoad`)))
  (if (== CalledTag (`self.Tag to bind Open`))
    (`self.OpenGrid`)
    (bind _value (`StructUtilsFunctionLibrary.GetInstancedStructValue` _saveddata :!label _label)
      (:`Valid`
        (bind _structout (setmembers `InteractableSavedData` :`StructRef` _value :`bIsConsummed` true))
        (`StructUtilsFunctionLibrary.SetInstancedStructValue` _saveddata _structout)
        (return false)))
    (elif (== CalledTag (`self.Tag to Bind Close`))
      (`self.CloseGrid`)
      (goto _label))))

(fn `UserConstructionScript`
  (if (`self.Turn`)
    (`SceneComponent.K2_SetRelativeRotation` (`self.SM_Grid_Staff_Door`) (`KismetMathLibrary.MakeRotator` 0.0 0.0 (`self.FinalRotation`)) false false)
    (else
      (`SceneComponent.K2_SetRelativeRotation` (`self.SM_Grid_Staff_Door`) (`KismetMathLibrary.MakeRotator` 0.0) false false))))