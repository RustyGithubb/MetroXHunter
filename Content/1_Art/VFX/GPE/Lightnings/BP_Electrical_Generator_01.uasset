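; BP_Electrical_Generator_01 is an electrical generator gameplay prop that plays visual effects when damaged or destroyed through its life component.
; On damage it spawns a jittering lightning ball actor at its LightningsPoint, fires the explosion effect, then destroys the ball after a short delay.
; On death it fires only the explosion effect, while leftover LightningElectricity activations remain unwired.
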(event `self.BP_LifeComponent.OnDeath`
  (params (DamageContext :type "/Game/0_Design/LifeSystem/Structs/F_DamageContext Structure"))
  (`ActorComponent.Activate` (`self.Generator_Explosion`) false))

(event `self.BP_LifeComponent.OnDamage`
  (params (DamageContext :type "/Game/0_Design/LifeSystem/Structs/F_DamageContext Structure"))
  (bind _returnvalue (`|SpawnActorFromClass` "/Game/1_Art/VFX/GPE/Lightnings/BP_Lightning_Ball_Jitter_GPE.BP_Lightning_Ball_Jitter_GPE_C" (`SceneComponent.K2_GetComponentToWorld` (`self.Lightnings_Point`)) "Undefined" "MultiplyWithRoot" null null))
  (`ActorComponent.Activate` (`self.Generator_Explosion`) false)
  (`KismetSystemLibrary.Delay` 1.0)
  (`self.K2_DestroyActor` _returnvalue))

(fn `UserConstructionScript`)