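; BP_AmbientSound is an ambient sound actor whose volume follows a light flicker effect.
; It caches the AudioComponent's volume multiplier at BeginPlay, scales it by IntensityScale on each flicker update, and restores it when flickering stops.
; The start and tick callbacks are empty, and RetrieveFlickableLights returns a PointLight, which a TODO marks as an unwanted workaround.
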(event `self.ReceiveBeginPlay`
  (set `self.DefaultVolumeMultiplier` (`AudioComponent.VolumeMultiplier` (`self.AudioComponent`))))

(fn `OnFlickLightStart`
  (params (LightData :type "LightData Structure (by ref)"))
  (return))

(fn `OnFlickLightStop`
  (params (LightData :type "LightData Structure (by ref)"))
  (`AudioComponent.SetVolumeMultiplier` (`self.AudioComponent`) (`self.DefaultVolumeMultiplier`))
  (return))

(fn `OnFlickLightTick`
  (params (DeltaTime :type "Float (single-precision)") (LightData :type "LightData Structure (by ref)"))
  (return))

(fn `OnFlickLightUpdate`
  (params (LightData :type "LightData Structure (by ref)") (IntensityScale :type "Float (single-precision)"))
  (`AudioComponent.SetVolumeMultiplier` (`self.AudioComponent`) (* (`self.DefaultVolumeMultiplier`) IntensityScale))
  (return))

(fn `RetrieveFlickableLights`
  (returns (ReturnValue :type "Array of LightComponent Object Reference"))
  (return (`|MakeArray` (`self.PointLight`) :!type "LightComponent Object Reference")) ; TODO: Find a way to not use this
)

(fn `UserConstructionScript`)