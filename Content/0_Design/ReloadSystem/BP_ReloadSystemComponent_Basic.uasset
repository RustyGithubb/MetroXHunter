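; Basic reload system component that refills the player gun's magazine after a timed reload and drives its ammo HUD.
; On BeginPlay it creates the reload widget, syncs it to current ammo and binds the gun's OnFire to remove a bullet.
; Reload input on a non-full magazine plays the widget animation, waits ReloadTime, then refills.
; The reloading flag blocks repeat reloads and is exposed through IsLockingGunFire.
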(event `self.ReceiveBeginPlay`
  ;[1 1 1] BEGINPLAY
  (`self.CreateWidget`)
  (`self.InitializeWidget`)
  (add `/Game/0_Design/GameManagement_/BP_Gun.OnFire` (`self.Gun`) (delegate `OnFire`)))

(event `OnFire`
  ;[1 1 1] ONFIRE
  (`/Game/UI/Widgets/WBP_ReloadSystem_Basic.RemoveBullet` (`self.Widget`)))

(event `ReloadEvent`
  (bind _gun (`self.Gun`))
  ;[1 1 1] RELOAD EVENT
  (if (not (`self.IsLockingGunFire`))
    (set `self.IsReloading` true)
    (`/Game/UI/Widgets/WBP_ReloadSystem_Basic.ReloadAnimation` (`self.Widget`) (`self.ReloadTime`))
    (`KismetSystemLibrary.Delay` (`self.ReloadTime`))
    (set `/Game/0_Design/GameManagement_/BP_Gun.IndexMagazineAmmo` (`/Game/0_Design/GameManagement_/BP_Gun.MaxMagazineAmmo` _gun) _gun)
    (set `self.IsReloading` false)))

(event `self.ReceiveEndPlay`
  (params (EndPlayReason :type "EEndPlayReason Enum" :default "Destroyed"))
  ;[1 1 1] ENDPLAY (Remove Widget)
  (bind _widget (`self.Widget`)
    (:`then`
      (`Widget.RemoveFromParent` _widget))
    (:`else`)))

(fn `CreateWidget`
  (bind _asbpc_controller (cast `/Game/0_Design/GameManagement_/BPC_Controller` (`Pawn.GetController` (`self.PlayerCharacter`))))
  (bind _returnvalue (`|CreateWidget` "/Game/UI/Widgets/WBP_ReloadSystem_Basic.WBP_ReloadSystem_Basic_C" _asbpc_controller))
  (bind _output_get (set `self.Widget` _returnvalue))
  (`UserWidget.AddToViewport` _output_get 0))

(fn `InitializeWidget`
  (bind _gun (`self.Gun`))
  (bind _indexmagazineammo (`/Game/0_Design/GameManagement_/BP_Gun.IndexMagazineAmmo` _gun))
  (bind _maxmagazineammo (`/Game/0_Design/GameManagement_/BP_Gun.MaxMagazineAmmo` _gun))
  (`self.Widget`
    (:`then`
      (if (< _indexmagazineammo _maxmagazineammo)
        (for _ (range 1 (+ (- _maxmagazineammo _indexmagazineammo) 1))
          (`/Game/UI/Widgets/WBP_ReloadSystem_Basic.RemoveBullet` (`self.Widget`)))))
    (:`else`)))

(fn `IsLockingGunFire`
  (returns (IsFireLocked :type Boolean))
  (return (`self.IsReloading`)))

(fn `OnReloadInput`
  (params (`Input Type` :type "/Game/0_Design/E_InputActionType Enum" :default "NewEnumerator0"))
  (switch `/Game/0_Design/E_InputActionType` `Input Type`
    (:`NewEnumerator1`
      (if (`/Game/0_Design/GameManagement_/BP_Gun.IsGunFull` (`self.Gun`))
        (`KismetSystemLibrary.PrintString` "Magazine Full!" true true (struct :`R` 1.0 :`G` 0.002279 :`A` 1.0))
        (else
          (`self.ReloadEvent`))))))