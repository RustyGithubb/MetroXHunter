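; Destructible smart-light traffic light that cycles through its green, orange and red lamp materials, advancing one step on each Tick.
; BeginPlay creates dynamic material instances from three static mesh slots.
; Each step resets those slots to black clear coat, then applies the current instance to the slot derived from the cycle index.
; The flicker update function is overridden to do nothing.
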(event `self.ReceiveBeginPlay`
  (`parent.ReceiveBeginPlay`)
  (bind _returnvalue (`KismetMaterialLibrary.CreateDynamicMaterialInstance` (`PrimitiveComponent.GetMaterial` (`self.StaticMesh`) 3)))
  (set `self.Green` _returnvalue)
  (bind _returnvalue_2 (`KismetMaterialLibrary.CreateDynamicMaterialInstance` (`PrimitiveComponent.GetMaterial` (`self.StaticMesh`) 2)))
  (set `self.Orange` _returnvalue_2)
  (bind _returnvalue_3 (`KismetMaterialLibrary.CreateDynamicMaterialInstance` (`PrimitiveComponent.GetMaterial` (`self.StaticMesh`) 1)))
  (set `self.Red` _returnvalue_3))

(event `self.ReceiveTick`
  (params (DeltaSeconds :type "Float (single-precision)"))
  (`self.Change light State` (`|GetArrayItem` (`|MakeArray` (`self.Green`) (`self.Orange`) (`self.Red`)) (`self.Index`)))
  (bind _result (`/Engine/EditorBlueprintResources/StandardMacros.IncrementInt` (`self.Index`))
    (:`  `
      (if (>= _result 3)
        (set `self.Index` 0)))))

(fn `Change light State`
  (params (Material :type "MaterialInterface Object Reference"))
  (for _index (range 1 4)
    (`PrimitiveComponent.SetMaterial` (`self.StaticMesh`) _index "/Engine/EditorMeshes/ColorCalibrator/M_ClearCoatBlack.M_ClearCoatBlack"))
  (`PrimitiveComponent.SetMaterial` (`self.StaticMesh`) (+ (`self.Index`) 1) Material))

(fn `OnFlickLightUpdate`
  (params (LightData :type "LightData Structure (by ref)") (IntensityScale :type "Float (single-precision)"))
  (return))

(fn `UserConstructionScript`
  (`parent.UserConstructionScript`))