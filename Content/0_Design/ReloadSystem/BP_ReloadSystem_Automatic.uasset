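; Automatic reload system that refills the player's gun magazine through an on-screen widget, created on BeginPlay with drain and block settings.
; Gun fire events drive the widget and flag the magazine as not full, so Tick refills it by a fixed per-frame amount, independent of delta time.
; Widget callbacks add one round to the gun on reload and stop the refill once the magazine is full.
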(event `self.ReceiveBeginPlay`
  (bind _widget (`self.Widget`))
  (bind _gun (`self.Gun`))
  (`self.CreateWidget`)
  (add `/Game/0_Design/GameManagement_/BP_Gun.OnFire` (`self.Gun`) (delegate `OnFire`))
  (add `/Game/UI/Widgets/WBP_ReloadSystem_Automatic.OnMagazineRefilled` _widget (delegate `OnMagazineRefilled`))
  (add `/Game/UI/Widgets/WBP_ReloadSystem_Automatic.OnReload` _widget (delegate `OnReload`))
  (set `/Game/0_Design/GameManagement_/BP_Gun.IndexMagazinAmmo` (`/Game/0_Design/GameManagement_/BP_Gun.MaxMagazinAmmo` _gun) _gun))

(event `OnFire`
  (`/Game/UI/Widgets/WBP_ReloadSystem_Automatic.OnFire` (`self.Widget`))
  (set `self.IsMagazineFull` false))

(event `OnMagazineRefilled`
  (set `self.IsMagazineFull` true))

(event `OnReload`
  (`/Engine/EditorBlueprintResources/StandardMacros.IncrementInt` (`/Game/0_Design/GameManagement_/BP_Gun.IndexMagazinAmmo` (`self.Gun`))))

(event `self.ReceiveTick`
  (params (DeltaSeconds :type "Float (single-precision)"))
  (if (not (`self.IsMagazineFull`))
    (`/Game/UI/Widgets/WBP_ReloadSystem_Automatic.RefillBullet` (`self.Widget`) 0.001)))

(fn `CreateWidget`
  (bind _asbpc_controller (cast `/Game/0_Design/GameManagement_/BPC_Controller` (`Pawn.GetController` (`self.PlayerCharacter`))))
  (bind _returnvalue (`|CreateWidget` "/Game/UI/Widgets/WBP_ReloadSystem_Automatic.WBP_ReloadSystem_Automatic_C" _asbpc_controller))
  (bind _output_get (set `self.Widget` _returnvalue))
  (set `/Game/UI/Widgets/WBP_ReloadSystem_Automatic.Drain Amount` (`self.Drain Amount`) _output_get)
  (set `/Game/UI/Widgets/WBP_ReloadSystem_Automatic.Block Amount` (`self.Block Amount`) _output_get)
  (`UserWidget.AddToViewport` _output_get 0))