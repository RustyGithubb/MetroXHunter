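; Swinging metal door that opens with a sound and yaw timeline, and closes when it receives a listened gameplay event.
; Box overlaps are passed to OnDoorHit; SetDoorOpened removes the interaction component and fires a gameplay event as the door swings.
; A second timeline handles closing, but also sets IsOpened to true when finished.
; The construction script uses FlipRotation to set swing direction, mesh offset and arrow orientation.
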(event `self.ReceiveBeginPlay`
  (bind (_relativerotation_roll _relativerotation_pitch _relativerotation_yaw) (`KismetMathLibrary.BreakRotator` (`SceneComponent.RelativeRotation` (`self.Door`))))
  (set `self.StartYawRotation` _relativerotation_yaw)
  (`/EventDispatcherHub/FunctionLibrary/BPL_EventDispatcherHub.Bind to Single Gameplay Event` (`self.Event to Listen`) self))

(event `self.Box.OnComponentBeginOverlap`
  (params (OverlappedComponent :type "PrimitiveComponent Object Reference") (OtherActor :type "Actor Object Reference") (OtherComp :type "PrimitiveComponent Object Reference") (OtherBodyIndex :type Integer) (bFromSweep :type Boolean) (SweepResult :type "HitResult Structure (by ref)"))
  (`self.OnDoorHit` OtherActor))

(event `self.SetDoorOpened`
  (params (bShouldOpen :type Boolean))
  (if bShouldOpen
    (`GameplayStatics.PlaySoundAtLocation` "/Game/Sounds/Audio/SFX/SFX_GPE/SFX_Door/SC_MetalDoor_Opening.SC_MetalDoor_Opening" (`SceneComponent.K2_GetComponentLocation` (`self.AudioPos`)) (struct) 1.0 1.0 0.0 null null null null)
    (`self.InteractableComponent`
      (:`then`
        (`self.SetInteractionFreezed` true)
        (`self.RemoveInteractionComponent`)
        (`/EventDispatcherHub/FunctionLibrary/BPL_EventDispatcherHub.Call Single Gameplay Event` (`self.Tag to Call`) self)
        (bind (_direction _rotation) (`Timeline|OpenDoor` :!via `PlayFromStart`)
          (:`Update`
            (`SceneComponent.K2_SetRelativeRotation` (`self.Door`) (`KismetMathLibrary.MakeRotator` 0.0 0.0 (+ (* _rotation (`self.FinalRotation`)) (`self.StartYawRotation`))) false false))
          (:`Finished`
            (set `self.bIsOpened` true))))
      (:`else`))))

(event `self.CloseDoorEditor`
  (bind (_direction _rotation) (`Timeline|Timeline` :!via `PlayFromStart` :!label _label)
    (:`Update`
      (`SceneComponent.K2_SetRelativeRotation` (`self.Door`) (`KismetMathLibrary.MakeRotator` 0.0 0.0 (`KismetMathLibrary.Lerp` (`self.FinalRotation`) (`self.StartYawRotation`) _rotation)) false false))
    (:`Finished`
      (set `self.bIsOpened` true))))

(event `Close`
  (goto _label :!via `PlayFromStart`))

(fn `ReceiveEvent`
  (params (CalledTag :type "GameplayTag Structure") (CallingObject :type "Object Object Reference (by ref)"))
  (returns (Return :type Boolean))
  (if (== CalledTag (`self.Event to Listen`))
    (`self.Close`)))

(fn `UserConstructionScript`
  (if (`self.bFlipRotation`)
    (set `self.FinalRotation` (`self.TargetRotation`))
    (`SceneComponent.K2_SetRelativeLocation` (`self.StaticMesh`) (0.0 -150.0 0.0) false false)
    (`SceneComponent.K2_SetRelativeRotation` :`self` (`self.Arrow`))
    (else
      (set `self.FinalRotation` (* (`self.TargetRotation`) -1.0))
      (`SceneComponent.K2_SetRelativeLocation` (`self.StaticMesh`) (-40.0 -150.0 0.0) false false)
      (`SceneComponent.K2_SetRelativeRotation` (`self.Arrow`) (struct :`Yaw` -180.0) false false))))