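; BP_AIAttackComponent is an enemy AI component that manages its owner's token reservations on an attack target.
; ReserveTarget stores the target and requests tokens from it with the owner as reserver, returning the result.
; FreeTarget and FreeAllTokens release tokens and clear the stored target, with each call logged under VisLogBP.
; On EndPlay it frees the owner's reservations on any still-valid target.
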(event `self.ReceiveEndPlay`
  (params (EndPlayReason :type "EEndPlayReason Enum" :default "Destroyed"))
  (bind _currentaitarget (`self.CurrentAITarget`)
    (:`then`
      (`/Game/Design/Enemies/AI/BP_AITargetComponent.FreeReservations` _currentaitarget (`self.GetOwner`)))
    (:`else`)))

(fn `FreeAllTokens`
  (bind _currentaitarget (`self.CurrentAITarget`)
    (:`then`
      (`/Game/Design/Enemies/AI/BP_AITargetComponent.FreeAllTokens` _currentaitarget (`self.GetOwner`))
      (set `self.CurrentAITarget` null)
      (`VisualLoggerKismetLibrary.LogText` null "FreeAllTokens" "VisLogBP" true))
    (:`else`)))

(fn `FreeTarget`
  (params (AITarget :type "/Game/Design/Enemies/AI/BP_AITargetComponent Object Reference") (Tokens :type Integer :default 1))
  (`/Game/Design/Enemies/AI/BP_AITargetComponent.FreeTokens` AITarget (`self.GetOwner`) Tokens)
  (set `self.CurrentAITarget` null)
  (`VisualLoggerKismetLibrary.LogText` null "FreeTokens" "VisLogBP" true))

(fn `ReserveTarget`
  (params (AITarget :type "/Game/Design/Enemies/AI/BP_AITargetComponent Object Reference") (Tokens :type Integer :default 1))
  (returns (bIsSuccess :type Boolean))
  (bind _output_get (set `self.CurrentAITarget` AITarget))
  (bind _bissuccess (`/Game/Design/Enemies/AI/BP_AITargetComponent.ReserveTokens` _output_get (`self.GetOwner`) Tokens))
  (`VisualLoggerKismetLibrary.LogText` null "ReserveTokens" "VisLogBP" true)
  (return _bissuccess))