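; BP_Elevator is an interactable elevator that travels vertically to a target location set relative to the actor.
; While its moving flag is set, Tick offsets it along negative local Z by its speed per frame, without delta-time scaling.
; Once within one step of the target, it stops and ends the interaction after a short delay.
; The construction script computes that world target and previews the path and destination with debug drawing.
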(event `self.ReceiveTick`
  (params (DeltaSeconds :type "Float (single-precision)"))
  (if (`self.bIsElevatorMoving`)
    (`self.K2_AddActorLocalOffset` (`KismetMathLibrary.MakeVector` 0.0 0.0 (* (`self.ElevatorSpeed`) -1.0)))
    (if (<= (`KismetMathLibrary.Vector_Distance` (`self.NextPosition`) (`SceneComponent.K2_GetComponentLocation` (`self.SceneRoot`))) (`self.ElevatorSpeed`))
      (set `self.bIsElevatorMoving` false)
      (`KismetSystemLibrary.Delay` 0.2)
      (`self.EndInteraction`))))

(fn `UserConstructionScript`
  (bind _returnvalue (`KismetMathLibrary.TransformLocation` (`self.GetTransform`) (`self.TargetLocation`)))
  ;[1 1 1] Draw Line
  (`KismetSystemLibrary.FlushPersistentDebugLines`)
  (set `self.NextPosition` _returnvalue)
  (`KismetSystemLibrary.DrawDebugLine` (`SceneComponent.K2_GetComponentLocation` (`self.StaticMesh`)) _returnvalue (struct :`A` 1.0) 10.0 10.0)
  (`KismetSystemLibrary.DrawDebugBox` _returnvalue (`.BoxExtent` (`KismetSystemLibrary.GetComponentBounds` (`self.StaticMesh`))) (struct :`R` 0.246902 :`G` 1.0 :`A` 1.0) (struct) 10.0 10.0))