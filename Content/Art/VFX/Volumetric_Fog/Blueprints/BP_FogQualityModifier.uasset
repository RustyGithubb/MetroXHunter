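; Trigger volume that changes volumetric fog quality while the player character is inside it.
; On BeginPlay it caches the current fog GridSizeZ and GridPixelSize console variables.
; Player overlap issues console commands from the selected quality tier, and exit issues them with the cached values, affecting fog globally.
; The construction script picks a cube or sphere mesh, and a debug flag shows the volume and icon and prints messages.
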(event `self.ReceiveBeginPlay`
  (`self.GetFogDefaultQuality`)
  (`self.Debug`))

(event `self.SM.OnComponentBeginOverlap`
  (params (OverlappedComponent :type "PrimitiveComponent Object Reference") (OtherActor :type "Actor Object Reference") (OtherComp :type "PrimitiveComponent Object Reference") (OtherBodyIndex :type Integer) (bFromSweep :type Boolean) (SweepResult :type "HitResult Structure (by ref)"))
  (`self.CheckPlayer` OtherActor)
  (`self.SetFogQuality`)
  (`self.DebugMessage` :!label _label))

(event `self.SM.OnComponentEndOverlap`
  (params (OverlappedComponent :type "PrimitiveComponent Object Reference") (OtherActor :type "Actor Object Reference") (OtherComp :type "PrimitiveComponent Object Reference") (OtherBodyIndex :type Integer))
  (`self.CheckPlayer` OtherActor)
  (`self.ResetFogQuality`)
  (goto _label :!via `Exit`))

(fn `Debug`
  (if (`self.IsDebug`)
    (`SceneComponent.SetHiddenInGame` (`self.SM`) false false)
    (`SceneComponent.SetHiddenInGame` (`self.Icon`) false false)
    (else
      (`SceneComponent.SetHiddenInGame` (`self.Icon`) true false)
      (`SceneComponent.SetHiddenInGame` (`self.SM`) true false))))

(fn `FogQualityGridSizeZ`
  (returns (NewParam :type String))
  (bind (_qualityvariables_gridpixelsize _qualityvariables_gridsizez) (break `/Game/Art/VFX/Volumetric_Fog/Struct/F_FogQualityVariables` (`self.QualityVariables`)))
  (return (`KismetStringLibrary.Concat_StrStr` "r.VolumetricFog.GridSizeZ" "" (select `/Game/Art/VFX/Volumetric_Fog/Enum/E_FogQuality` (`self.Quality`) :`NewEnumerator0` (`|GetArrayItem` _qualityvariables_gridsizez) :`NewEnumerator1` (`|GetArrayItem` _qualityvariables_gridsizez 1) :`NewEnumerator2` (`|GetArrayItem` _qualityvariables_gridsizez 2) :`NewEnumerator3` (`|GetArrayItem` _qualityvariables_gridsizez 3)))))

(fn `FogQualityPixelSize`
  (returns (ReturnValue :type String))
  (bind _qualityvariables_gridpixelsize (break `/Game/Art/VFX/Volumetric_Fog/Struct/F_FogQualityVariables` (`self.QualityVariables`)))
  (return (`KismetStringLibrary.Concat_StrStr` "r.VolumetricFog.GridPixelSize" "" (select `/Game/Art/VFX/Volumetric_Fog/Enum/E_FogQuality` (`self.Quality`) :`NewEnumerator0` (`|GetArrayItem` _qualityvariables_gridpixelsize) :`NewEnumerator1` (`|GetArrayItem` _qualityvariables_gridpixelsize 1) :`NewEnumerator2` (`|GetArrayItem` _qualityvariables_gridpixelsize 2) :`NewEnumerator3` (`|GetArrayItem` _qualityvariables_gridpixelsize 3)))))

(fn `GetFogDefaultQuality`
  (bind _returnvalue (`KismetSystemLibrary.GetConsoleVariableFloatValue` "r.VolumetricFog.GridSizeZ"))
  (set `self.GridSizeZ` _returnvalue)
  (bind _returnvalue_2 (`KismetSystemLibrary.GetConsoleVariableFloatValue` "r.VolumetricFog.GridPixelSize"))
  (set `self.GridPixelSize` _returnvalue_2))

(fn `ResetFogQuality`
  (`KismetSystemLibrary.ExecuteConsoleCommand` (`KismetStringLibrary.Concat_StrStr` "r.VolumetricFog.GridSizeZ" "" (`KismetStringLibrary.Conv_DoubleToString` (`self.GridSizeZ`))) null)
  (`KismetSystemLibrary.ExecuteConsoleCommand` (`KismetStringLibrary.Concat_StrStr` "r.VolumetricFog.GridPixelSize" "" (`KismetStringLibrary.Conv_DoubleToString` (`self.GridPixelSize`))) null))

(fn `SetFogQuality`
  (`KismetSystemLibrary.ExecuteConsoleCommand` (`self.FogQualityGridSizeZ`) null)
  (`KismetSystemLibrary.ExecuteConsoleCommand` (`self.FogQualityPixelSize`) null))

(fn `UserConstructionScript`
  (`StaticMeshComponent.SetStaticMesh` (`self.SM`) (select `/Game/Art/VFX/Volumetric_Fog/Enum/E_CollisionType` (`self.CollisionShape`) :`NewEnumerator0` "/Game/Art/VFX/Volumetric_Fog/Meshes/SM_FogCube.SM_FogCube" :`NewEnumerator1` "/Game/Art/VFX/Volumetric_Fog/Meshes/SM_FogSphere.SM_FogSphere" :!type "StaticMesh Object Reference")))