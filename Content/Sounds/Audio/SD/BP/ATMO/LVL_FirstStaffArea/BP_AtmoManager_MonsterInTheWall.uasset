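; Level audio manager for the monster-in-the-wall atmosphere in the First Staff Area, driven by Start and End overlap volumes.
; When the player pawn enters Start, it assigns the looping MetaSound to MSAtmoManager and plays it.
; Entering End sends the MetaSound an "End" trigger parameter.
; Each volume has its own Gate that closes after firing, so each fires only once.
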(event `self.Start.OnComponentBeginOverlap`
  (params (OverlappedComponent :type "PrimitiveComponent Object Reference") (OtherActor :type "Actor Object Reference") (OtherComp :type "PrimitiveComponent Object Reference") (OtherBodyIndex :type Integer) (bFromSweep :type Boolean) (SweepResult :type "HitResult Structure (by ref)"))
  (bind _ms_atmomanager (`self.MS_AtmoManager`))
  ;[1 1 1 0.33] IN
  (if (== OtherActor (`GameplayStatics.GetPlayerPawn` 0))
    (`/Engine/EditorBlueprintResources/StandardMacros.Gate` false :!label _label
      (:`Exit`
        (`AudioComponent.SetSound` _ms_atmomanager "/Game/Sounds/Audio/SD/MetaSounds/MS_Sources/ATMO/LVL_FirstStaffArea/MS_ATMO_FirstStaffArea_MonsterInTheWall.MS_ATMO_FirstStaffArea_MonsterInTheWall") ; NOTE: The sound asset must have "Looping" set to true
        (`AudioComponent.Play` _ms_atmomanager 0.0)
        (goto _label :!via `Close`)))))

(event `self.End.OnComponentBeginOverlap`
  (params (OverlappedComponent :type "PrimitiveComponent Object Reference") (OtherActor :type "Actor Object Reference") (OtherComp :type "PrimitiveComponent Object Reference") (OtherBodyIndex :type Integer) (bFromSweep :type Boolean) (SweepResult :type "HitResult Structure (by ref)"))
  ;[1 1 1 0.33] OUT
  (if (== OtherActor (`GameplayStatics.GetPlayerPawn` 0))
    (`/Engine/EditorBlueprintResources/StandardMacros.Gate` false :!label _label_2
      (:`Exit`
        (`AudioParameterControllerInterface.SetTriggerParameter` (`self.MS_AtmoManager`) "End")
        (goto _label_2 :!via `Close`)))))

(fn `UserConstructionScript`)