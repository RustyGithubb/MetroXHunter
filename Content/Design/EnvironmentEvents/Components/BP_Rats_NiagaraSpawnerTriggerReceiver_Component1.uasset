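; Trigger receiver component that plays a rat Niagara effect at an offset from its owning actor in environment events.
; On BeginPlay it pre-spawns the inactive, hidden system to avoid activation stutter, passing in player repulse radius and rat spawn rate.
; The component-specific play event reveals and activates that pooled system.
; A debug function draws axis arrows to preview the spawn location and rotation.
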(event `self.ReceiveBeginPlay`
  (`self.PoolNiagara`))

(fn `DisplayNiagaraLocation`
  (locals (ArrowStart :type "Vector Structure" :default (0.0 0.0 0.0)))
  (bind _arrowstart (`local.ArrowStart`))
  (bind _arrowstart_2 (`local.ArrowStart`))
  (bind _arrowstart_3 (`local.ArrowStart`))
  (`KismetSystemLibrary.FlushPersistentDebugLines`)
  (set `local.ArrowStart` (+ (`Actor.K2_GetActorLocation` (`self.GetOwner`)) (`self.NiagaraWorldLocationOffSet`)))
  (`KismetSystemLibrary.DrawDebugArrow` _arrowstart_2 (+ _arrowstart_2 (* (`KismetMathLibrary.GetForwardVector` (`self.NiagaraWorldRotation`)) 50.0)) 10.0 (struct :`R` 1.0 :`A` 1.0) 10.0 2.0)
  (`KismetSystemLibrary.DrawDebugArrow` _arrowstart_3 (+ _arrowstart_3 (* (`KismetMathLibrary.GetRightVector` (`self.NiagaraWorldRotation`)) 50.0)) 10.0 (struct :`G` 1.0 :`A` 1.0) 10.0 2.0)
  (`KismetSystemLibrary.DrawDebugArrow` _arrowstart (+ _arrowstart (* (`KismetMathLibrary.GetUpVector` (`self.NiagaraWorldRotation`)) 50.0)) 10.0 (struct :`B` 1.0 :`A` 1.0) 10.0 2.0))

(fn `OnPlayComponentSpecificEvent`
  (params (FromBoxEnter :type Boolean) (TriggerBox :type "Actor Object Reference"))
  (`/Engine/EditorBlueprintResources/StandardMacros.IsValid` (`self.SpawnedNiagara`)
    (:`Is Valid`
      (`SceneComponent.SetVisibility` (`self.SpawnedNiagara`) true false)
      (`self.Activate` (`self.SpawnedNiagara`) true))))

(fn `PoolNiagara`
  ;[0.06337 0.106 0.1823 0.33] Pool the Niagara to avoid any stutter when it needs to activate
  (bind _returnvalue (`NiagaraFunctionLibrary.SpawnSystemAtLocation` (`self.System Template`) (+ (`Actor.K2_GetActorLocation` (`self.GetOwner`)) (`self.NiagaraWorldLocationOffSet`)) (`self.NiagaraWorldRotation`) (1.0 1.0 1.0) true false))
  (`PrimitiveComponent.SetCastShadow` _returnvalue true)
  (`NiagaraComponent.SetVariableFloat` _returnvalue "PlayerRepulseRadius" (`self.Player Repulse Radius`))
  (`NiagaraComponent.SetVariableFloat` _returnvalue "Rats Spawn Rate" (`self.Rats Spawn Rate`))
  (bind _output_get (set `self.SpawnedNiagara` _returnvalue))
  (`SceneComponent.SetVisibility` _output_get false false)
  (`NiagaraComponent.SetAutoDestroy` _returnvalue false))