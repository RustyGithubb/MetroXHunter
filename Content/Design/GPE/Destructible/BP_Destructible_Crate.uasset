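; Destructible crate actor that bursts into fragments and may drop a random pickup when its Health component reports death.
; It removes the cube mesh, then spawns crate pieces at random cube-corner offsets, with impulses following the horizontal hit direction plus scatter and lift.
; Loot is a weighted pick, async-loaded, ground-snapped by a downward trace and given a random amount in its range.
; The actor destroys itself once loot spawns or none is valid.
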(event `self.Health.OnDeath`
  (params (DamageContext :type "DamageContext Structure (by ref)"))
  (`ActorComponent.K2_DestroyComponent` (`self.Cube`)) ; To be sure the spawned Debris don't\nget a wild rotation or location
  (for _ (range 8)
    (`self.SpawnCrateFragment` DamageContext))
  (`self.SpawnLoot`
    (:`Execute_PostLoad`
      _)
    (:`Execute_NoSpawn`
      _))
  (`self.K2_DestroyActor`))

(fn `SpawnCrateFragment`
  (params (DamageContext :type "DamageContext Structure (by ref)"))
  (bind _returnvalue_location (`KismetMathLibrary.BreakTransform` (`self.GetTransform`)))
  (bind (_bblockinghit _binitialoverlap _time _distance _location _impactpoint _normal _impactnormal _physmat _hitactor _hitcomponent _hitbonename _bonename _hititem _elementindex _faceindex _tracestart _traceend) (`GameplayStatics.BreakHitResult` DamageContext_HitResult))
  (bind (_returnvalue_x _returnvalue_y) (`KismetMathLibrary.BreakVector` (- _traceend _tracestart)))
  (`|SpawnActorFromClass` "/Game/Design/GPE/Destructible/BP_CratePiece.BP_CratePiece_C" (`KismetMathLibrary.MakeTransform` (+ _returnvalue_location (`KismetMathLibrary.MakeVector` (* (`KismetMathLibrary.RandomInteger` 2) 100) (* (`KismetMathLibrary.RandomInteger` 2) 100) (* (`KismetMathLibrary.RandomInteger` 2) 100))) (`KismetMathLibrary.RandomRotator` true)) "Undefined" "MultiplyWithRoot" null (`KismetMathLibrary.Normal` (+ (`KismetMathLibrary.Normal` (`KismetMathLibrary.MakeVector` _returnvalue_x _returnvalue_y)) (`KismetMathLibrary.MakeVector` (* (`KismetMathLibrary.RandomFloatInRange` -1.0 1.0) 0.4) (* (`KismetMathLibrary.RandomFloatInRange` -1.0 1.0) 0.4) 0.7))) null))

(fn `UserConstructionScript`)