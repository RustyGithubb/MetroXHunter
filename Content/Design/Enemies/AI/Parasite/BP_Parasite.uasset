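; Parasite enemy that possesses corpses and travels through vents, with materials taken from its data asset.
; Timelines drive the wiggling lunge into a corpse and the slides in and out of vents.
; Death halts possession and vent entry, fades wart glow using damage-type curves, and clears ShouldSpawn so loading destroys it; otherwise loading restores its transform.
; Bullet, melee and explosion hits add traced blood decals to the parent splash.
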(event `self.SaveComponent.OnSaveActor`
  (bind _saveddata (`SaveLoadComponent.SavedData` (`self.SaveComponent`)))
  ;[0 0.5104 1 0.33] ON SAVE
  (bind _value (`StructUtilsFunctionLibrary.GetInstancedStructValue` _saveddata)
    (:`Valid`
      (bind _structout (setmembers `BaseSavedData` :`StructRef` _value :`LastLocation` (`self.GetTransform`) :`bShouldSpawn` (`self.Should Spawn`)))
      (`StructUtilsFunctionLibrary.SetInstancedStructValue` _saveddata _structout))))

(event `self.SaveComponent.OnLoadActor`
  ;[0 1 0.05748 0.33] ON LOAD
  (bind _value (`StructUtilsFunctionLibrary.GetInstancedStructValue` (`SaveLoadComponent.SavedData` (`self.SaveComponent`)))
    (:`Valid`
      (bind (_lastlocation _bshouldspawn) (break `BaseSavedData` _value))
      (if _bshouldspawn
        (`self.K2_SetActorTransform` _lastlocation)
        (else
          (`self.K2_DestroyActor`))))))

(event `self.ReceiveBeginPlay`
  (bind _savecomponent (`self.SaveComponent`))
  (bind _mesh (`self.Mesh`))
  (bind _dataasset (`self.DataAsset`))
  (`|ExecutionSequence`
    (:`then_0`
      ;[0 1 0.05748 0.33] Initialize Components to save
      (`KismetArrayLibrary.Array_Add` (`SaveLoadComponent.ComponentsToSave` (`self.SaveComponent`)) (`self.HealthComponent`))
      ;[0 1 0.05748 0.33] Force Load if the Actor is initialized too late on the level streaming
      (if (not (`SaveLoadComponent.bIsDataLoaded` _savecomponent))
        (`SaveLoadComponent.Load` _savecomponent)))
    (:`then_1`
      (`PrimitiveComponent.SetMaterial` _mesh 0 (`ParasiteData.BodyMaterial` _dataasset))
      (`PrimitiveComponent.SetMaterial` _mesh 1 (`ParasiteData.WartsMaterial` _dataasset)))))

(event `self.StartPossessingCorpse`
  (params (Corpse :type "PossessableCorpse Object Reference"))
  (bind (_startanimtransform_location _startanimtransform_rotation) (`KismetMathLibrary.BreakTransform` (`self.StartAnimTransform`)))
  (bind _startanimtransform_location_2 (`KismetMathLibrary.BreakTransform` (`self.StartAnimTransform`)))
  (set `self.StartAnimTransform` (`KismetMathLibrary.MakeTransform` (`self.K2_GetActorLocation`) (`SceneComponent.RelativeRotation` (`self.Mesh`))))
  (bind (_direction _time _ratio) (`Timeline|PossessAnimationTimeline` :!via `PlayFromStart` :!label _label)
    (:`Update`
      ;[1 1 1 0.33] Parasite Animation
      (`SceneComponent.K2_SetRelativeRotation` (`self.Mesh`) (`KismetMathLibrary.ComposeRotators` _startanimtransform_rotation (`KismetMathLibrary.MakeRotator` 0.0 0.0 (* (`KismetMathLibrary.Sin` (* _time 20.0)) 20.0))) false false)
      (`self.K2_SetActorLocation` (`KismetMathLibrary.VLerp` _startanimtransform_location_2 (`self.K2_GetActorLocation` Corpse) _ratio)))
    (:`Finished`
      (`self.PossessCorpse` Corpse)
      (`self.OnPossessEnd`))))

(event `self.HealthComponent.OnDeath`
  (params (DamageContext :type "DamageContext Structure (by ref)"))
  (bind _startanimtransform (`self.StartAnimTransform`))
  (`|ExecutionSequence`
    (:`then_0`
      (goto _label :!via `Stop`))
    (:`then_1`
      (bind (_direction _time) (`Timeline|EnterVentAnimationTimeline` :!via `Stop` :!label _label_2)
        (:`Update`
          (bind (_returnvalue_x _returnvalue_y) (`KismetMathLibrary.BreakVector` (`SceneComponent.K2_GetComponentLocation` (`Vent.GetSpawnPointComponent` (stale `self.StartEnteringVent` Vent)))))
          (`self.K2_SetActorLocation` (`KismetMathLibrary.VLerp` (`KismetMathLibrary.MakeVector` (.x (.location _startanimtransform)) (.y (.location _startanimtransform)) (.z (.location _startanimtransform))) (`KismetMathLibrary.MakeVector` _returnvalue_x _returnvalue_y (.z (.location _startanimtransform))) _time)))
        (:`Finished`
          (`Vent.EnterVent` (stale `self.StartEnteringVent` Vent) self))
        (:`PlaySound`
          (`Vent.PlayEnterSound` (stale `self.StartEnteringVent` Vent)))))
    (:`then_2`
      (`self.DoFadeWarts` DamageContext))
    (:`then_3`
      (set `self.Should Spawn` false))))

(event `self.StartEnteringVent`
  (params (Vent :type "Vent Object Reference"))
  (`Vent.StartEnterVent` Vent self)
  (set `self.StartAnimTransform` (`KismetMathLibrary.MakeTransform` (`self.K2_GetActorLocation`) (`SceneComponent.RelativeRotation` (`self.Mesh`))))
  (goto _label_2 :!via `PlayFromStart`))

(event `self.StartExitingVent`
  (params (Vent :type "Vent Object Reference"))
  (bind (_returnvalue_x _returnvalue_y) (`KismetMathLibrary.BreakVector` (`self.K2_GetActorLocation`)))
  (bind (_returnvalue_x_2 _returnvalue_y_2 _returnvalue_z) (`KismetMathLibrary.BreakVector` (`self.K2_GetActorLocation` Vent)))
  (bind _startanimtransform (`self.StartAnimTransform`))
  (bind (_returnvalue_x_3 _returnvalue_y_3) (`KismetMathLibrary.BreakVector` (`SceneComponent.K2_GetComponentLocation` (`Vent.GetEntranceComponent` Vent))))
  (set `self.StartAnimTransform` (`KismetMathLibrary.MakeTransform` (`KismetMathLibrary.MakeVector` _returnvalue_x _returnvalue_y (+ _returnvalue_z (`CapsuleComponent.CapsuleHalfHeight` (`self.CapsuleComponent`)))) (`SceneComponent.RelativeRotation` (`self.Mesh`))))
  (bind (_direction _time) (`Timeline|ExitVentAnimationTimeline` :!via `PlayFromStart`)
    (:`Update`
      (`self.K2_SetActorLocation` (`KismetMathLibrary.VLerp` (`KismetMathLibrary.MakeVector` (.x (.location _startanimtransform)) (.y (.location _startanimtransform)) (.z (.location _startanimtransform))) (`KismetMathLibrary.MakeVector` _returnvalue_x_3 _returnvalue_y_3 (.z (.location _startanimtransform))) _time)))))

(event `self.ElectrocutableComponent.OnElectricStart`
  (params (Duration :type "Float (single-precision)"))
  (bind _electrocutablecomponent (`self.ElectrocutableComponent`))
  (set `ElectrocutableComponent.FXAttachmentComponents` (`|MakeArray` (`self.Mesh`) :!type "SceneComponent Object Reference") _electrocutablecomponent)
  (set `ElectrocutableComponent.GigglingSkeletalComponents` (`|MakeArray` (`self.Mesh`)) _electrocutablecomponent))

(event `DoFadeWarts`
  (params (DamageContext :type "DamageContext Structure (by ref)"))
  (bind _mesh (`self.Mesh`))
  ;[1 1 1 0.33 32] Fade Warts animation
  (bind _returnvalue (`PrimitiveComponent.CreateDynamicMaterialInstance` _mesh 1 (`PrimitiveComponent.GetMaterial` _mesh 1) "None")) ; TODO: Think whether this should stay as is for optimization
  (bind _returnvalue_2 (`MaterialInstanceDynamic.K2_GetScalarParameterValue` _returnvalue "WartsEmissivePower"))
  (`TimelineComponent.SetPlayRate` (`self.FadeOutBulbTimeline`) (`KismetMathLibrary.RandomFloatInRange` 0.7 1.3))
  (bind (_direction _generic _shock _bullet) (`Timeline|FadeOutBulbTimeline` :!via `PlayFromStart`)
    (:`Update`
      (`MaterialInstanceDynamic.SetScalarParameterValue` _returnvalue "WartsEmissivePower" (* _returnvalue_2 (select `EDamageType` (`.DamageType` (break `DamageContext` DamageContext)) :`Generic` _generic :`Bullet` _bullet :`Melee` _generic :`Shock` (* _shock (`KismetMathLibrary.RandomFloatInRange` 0.5 1.5)) :`Explosion` _bullet :!type "Float (double-precision)")))
      (`SkeletalMeshComponent.SetAnimInstanceClass` (`self.Mesh`) null))))

(event `DoInstantBloodSplash`
  (params (DamageContext :type "DamageContext Structure (by ref)"))
  (bind (_healthcomponent _damageamount _damagetype _attackeractor _inflictoractor _hitresult) (break `DamageContext` DamageContext))
  (bind (_bblockinghit _binitialoverlap _time _distance _location _impactpoint _normal _impactnormal _physmat _hitactor _hitcomponent _hitbonename _bonename _hititem _elementindex _faceindex _tracestart _traceend) (`GameplayStatics.BreakHitResult` _hitresult))
  ;[1 1 1 0.33] Instant Blood Splash
  (if _bblockinghit
    (switch `EDamageType` _damagetype
      (:`Bullet`
        _)
      (:`Melee`
        _)
      (:`Explosion`
        _))
    (bind _outhit (`KismetSystemLibrary.LineTraceSingle` (+ _tracestart (* (`KismetMathLibrary.Vector_Up`) 35.0)) _traceend "TraceTypeQuery1" false (`|MakeArray` _attackeractor _inflictoractor)))
    (bind (_bblockinghit_2 _binitialoverlap_2 _time_2 _distance_2 _location_2 _impactpoint_2 _normal_2) (`GameplayStatics.BreakHitResult` _outhit))
    (`|SpawnActorFromClass` "/Game/Art/VFX/GPE/Decal/BP_Blood_Puddle_Decal.BP_Blood_Puddle_Decal_C" (`KismetMathLibrary.MakeTransform` _location_2 (`KismetMathLibrary.Conv_VectorToRotator` _normal_2) (* (`ParasiteData.BloodPuddleScale` (`self.DataAsset`)) (`self.GetActorScale3D`) 1.3)) "AlwaysSpawn" "MultiplyWithRoot" null false 0.0 2.0 (1.0 1.0 1.0) null)))

(event `self.EmitBloodSplash`
  (params (DamageContext :type "DamageContext Structure (by ref)"))
  (`parent.EmitBloodSplash` DamageContext)
  (`self.DoInstantBloodSplash` DamageContext))

(fn `UserConstructionScript`)