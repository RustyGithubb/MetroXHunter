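; Sound manager component for the Parasite enemy, handling its movement, damage, death, electrocution and bite QTE audio.
; BeginPlay binds to the owner's health, electrocution and bite events, which play one-shot screams or swap loops on its Audio component.
; Tick switches move and idle loops from grounded velocity unless electrocuted, and stops on death.
; The QTE plays as a 2D sound ended by success or fail triggers; footsteps are disconnected.
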(event `self.ReceiveBeginPlay`
  (bind _parasite (`self.Parasite`))
  (bind _electrocutablecomponent (`Parasite.ElectrocutableComponent` (`self.Parasite`)))
  ;[1 1 1 0.33] Bind to HealthComponent's events
  (bind _output_get (set `self.Parasite` (cast `/Game/Design/Enemies/AI/Parasite/BP_Parasite` (`self.GetOwner`) :!pure true)))
  (bind _healthcomponent (`Parasite.HealthComponent` _output_get))
  (add `HealthComponent.OnDamage` _healthcomponent (`|CreateDelegate` :!event `OnDamage`))
  (add `HealthComponent.OnDeath` _healthcomponent (`|CreateDelegate` :!event `OnDeath`))
  ;[1 1 1 0.33] Bind to ElectrocutableComponent events
  (add `ElectrocutableComponent.OnElectricStart` _electrocutablecomponent (`|CreateDelegate` :!event `OnElectricityStart`))
  (add `ElectrocutableComponent.OnElectricEnd` _electrocutablecomponent (`|CreateDelegate` :!event `OnElectricityEnd`))
  (add `/Game/Design/Enemies/AI/Parasite/BP_Parasite.OnBiteStarted` _parasite (`|CreateDelegate` :!event `OnQTEStarted`))
  (add `/Game/Design/Enemies/AI/Parasite/BP_Parasite.OnBiteFinished` _parasite (`|CreateDelegate` :!event `OnQTEFinished`)))

(event `self.OnScream`
  ;[1 0 0.06996 0.33 32] SCREAM
  (`GameplayStatics.PlaySoundAtLocation` "/Game/Sounds/Audio/SD/MetaSounds/MS_Sources/Ennemies/Parasites/MS_EnemySmall_Scream.MS_EnemySmall_Scream" (`Actor.K2_GetActorLocation` (`self.GetOwner`)) (struct) 1.0 1.0 0.0 null null null null))

(event `self.OnFootstep`
  ;[0 1 0.9332 0.33 32] FOOTSTEPS
)

(event `OnStartMoving`
  (bind _audio (`/Game/Design/Enemies/AI/Parasite/BP_Parasite.Audio` (`self.Parasite`)))
  ;[0 1 0.9332 0.33 32] MOVEMENT
  (`AudioComponent.SetSound` _audio "/Game/Sounds/Audio/SD/MetaSounds/MS_Sources/Ennemies/Parasites/MS_EnemySmall_Move_LP.MS_EnemySmall_Move_LP") ; TODO: Put the Movement sound loop
  (`AudioComponent.Play` _audio 0.0))

(event `OnStopMoving`
  (bind _audio (`/Game/Design/Enemies/AI/Parasite/BP_Parasite.Audio` (`self.Parasite`)))
  ;[0 1 0.9332 0.33 32] MOVEMENT
  (`AudioComponent.SetSound` _audio "/Game/Sounds/Audio/SD/MetaSounds/MS_Sources/Ennemies/Parasites/MS_EnemySmall_Idle_LP.MS_EnemySmall_Idle_LP") ; TODO: Put the Idle sound loop
  (`AudioComponent.Play` _audio 0.0))

(event `OnElectricityStart`
  (params (Duration :type "Float (single-precision)"))
  (bind _audio (`/Game/Design/Enemies/AI/Parasite/BP_Parasite.Audio` (`self.Parasite`)))
  ;[1 0 0 0.33 32] ELECTRICITY
  (if (and (not (`self.bIsElectrocuting`)) (`HealthComponent.IsAlive` (`Parasite.HealthComponent` (`self.Parasite`))))
    (`AudioComponent.SetSound` _audio "/Game/Sounds/Audio/SD/MetaSounds/MS_Sources/Ennemies/Parasites/MS_EnemySmall_Damage_LP.MS_EnemySmall_Damage_LP")
    (`AudioComponent.Play` _audio 0.0)
    (set `self.bIsElectrocuting` true)
    (set `self.bIsMoving` false)))

(event `OnDamage`
  (params (DamageContext :type "DamageContext Structure (by ref)"))
  ;[1 0 0 0.33 32] DAMAGE & DEATH
  (if (`HealthComponent.IsAlive` (`Parasite.HealthComponent` (`self.Parasite`)))
    (`GameplayStatics.PlaySoundAtLocation` "/Game/Sounds/Audio/SD/MetaSounds/MS_Sources/Ennemies/Parasites/MS_EnemySmall_Scream.MS_EnemySmall_Scream" (`Actor.K2_GetActorLocation` (`self.GetOwner`)) (struct) 1.0 1.0 0.0 null null null null)))

(event `OnElectricityEnd`
  ;[1 0 0 0.33 32] ELECTRICITY
  (if (`HealthComponent.IsAlive` (`Parasite.HealthComponent` (`self.Parasite`)))
    (`AudioComponent.FadeOut` (`/Game/Design/Enemies/AI/Parasite/BP_Parasite.Audio` (`self.Parasite`)) 1.0 0.0 "Linear")
    (set `self.bIsElectrocuting` false)))

(event `OnDeath`
  (params (DamageContext :type "DamageContext Structure (by ref)"))
  ;[1 0 0 0.33 32] DAMAGE & DEATH
  (`GameplayStatics.PlaySoundAtLocation` "/Game/Sounds/Audio/SD/MetaSounds/MS_Sources/Ennemies/Parasites/MS_EnemySmall_Death.MS_EnemySmall_Death" (`Actor.K2_GetActorLocation` (`self.GetOwner`)) (struct) 1.0 1.0 0.0 null null null null)
  (`AudioComponent.FadeOut` (`/Game/Design/Enemies/AI/Parasite/BP_Parasite.Audio` (`self.Parasite`)) 0.5 0.0 "Linear")
  (`self.SetComponentTickEnabled` false))

(event `self.ReceiveTick`
  (params (DeltaSeconds :type "Float (single-precision)"))
  (bind _parasite (`self.Parasite`))
  ;[1 1 1 0.33] Movement detection
  (if (and (> (`KismetMathLibrary.VSize` (`Actor.GetVelocity` _parasite)) 50.0) (`NavMovementComponent.IsMovingOnGround` (`Character.CharacterMovement` _parasite)) (not (`self.bIsElectrocuting`)))
    (if (not (`self.bIsMoving`))
      (set `self.bIsMoving` true)
      (`self.OnStartMoving`))
    (elif (`self.bIsMoving`)
      (set `self.bIsMoving` false)
      (`self.OnStopMoving`))))

(event `OnQTEStarted`
  (bind _returnvalue (`GameplayStatics.SpawnSound2D` "/Game/Sounds/Audio/SD/MetaSounds/MS_Sources/Ennemies/Parasites/MS_Parasite_QTE.MS_Parasite_QTE" 1.0 1.0 0.0 null))
  (set `self.AudioQTE` _returnvalue))

(event `OnQTEFinished`
  (params (bHasWon :type Boolean))
  (bind _audioqte (`self.AudioQTE`)
    (:`then`
      (`AudioParameterControllerInterface.SetTriggerParameter` _audioqte (`KismetMathLibrary.SelectName` "QTE_Success" "QTE_Fail" bHasWon)))
    (:`else`)))