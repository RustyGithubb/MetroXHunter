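; Gameplay setting unit that shows or hides the circle cursor of the shooting reticle.
; When the setting is applied in-game, it finds the first WBP_CursorShoot widget and caches it while it remains valid.
; The setting's boolean value switches that widget's CircleCursor between Visible and Collapsed.
; Applying the setting outside of gameplay does nothing.
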(event `self.OnApplySetting`
  (params (bInGame :type Boolean))
  (bind _wbp_cursorshoot (`self.WBP_CursorShoot`))
  (bind _circlecursor (`/Game/Design/Widgets/WBP_CursorShoot.CircleCursor` _wbp_cursorshoot))
  (if bInGame
    (`/Engine/EditorBlueprintResources/StandardMacros.IsValid` _wbp_cursorshoot
      (:`Is Valid`
        _)
      (:`Is Not Valid`
        (bind _foundwidgets (`WidgetBlueprintLibrary.GetAllWidgetsOfClass` "/Game/Design/Widgets/WBP_CursorShoot.WBP_CursorShoot_C" false))
        (set `self.WBP_CursorShoot` (`|GetArrayItem` _foundwidgets))))
    (if (`self.bValue`)
      (`Widget.SetVisibility` _circlecursor "Visible")
      (else
        (`Widget.SetVisibility` _circlecursor "Collapsed")))))