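; BP_Reload_QTE manages the gun's reload sequence; despite its QTE name, only the normal timed reload is implemented here.
; Reload input starts the sequence when the gun is idle and the magazine isn't full.
; A looping timer accumulates elapsed time until the normal duration, then clears itself and finalizes the reload, refilling ammo and returning to Idle.
; Reload sub-states currently only print debug strings.
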(event `self.ReceiveBeginPlay`
  (bind _gun (`self.Gun`))
  (set `self.Gun Reference` _gun)
  (`self.UpdateAmmoCount` (`/Game/0_Design/GameManagement_/BP_Gun.MaxMagazinAmmo` _gun)))

(event `StartReloadSequence`
  (set `self.CurrentGunState` "NewEnumerator2")
  (`self.UpdateCurrentReloadState` "NewEnumerator0")
  (set `self.ReloadElapsedTime` 0.0)
  (bind _returnvalue (`KismetSystemLibrary.K2_SetTimerDelegate` (delegate `UpdateReloadGauge`) (`self.ReloadRefreshRate`) true))
  (set `self.TimerHandleReloadPlayback` _returnvalue))

(event `UpdateReloadGauge`
  (set `self.ReloadElapsedTime` (+ (`self.ReloadElapsedTime`) (`self.ReloadRefreshRate`)))
  ;[1 1 1] Reload Normal si le joueur n'a pas appuyer pendant le timer
  (if (>= (`self.ReloadElapsedTime`) (`self.NormalReloadDuration`))
    (`KismetSystemLibrary.K2_ClearAndInvalidateTimerHandle` (`self.TimerHandleReloadPlayback`))
    (`self.TriggerNormalReload`)))

(event `TriggerNormalReload`
  (`self.FinalizeReload` (`/Game/0_Design/GameManagement_/BP_Gun.MaxMagazinAmmo` (`self.Gun Reference`)))
  (`self.UpdateCurrentReloadState` "NewEnumerator1"))

(fn `IsAmmoFull`
  (returns (ReturnValue :type Boolean))
  (bind _gun (`self.Gun`))
  (return (== (`/Game/0_Design/GameManagement_/BP_Gun.MaxMagazinAmmo` _gun) (`/Game/0_Design/GameManagement_/BP_Gun.IndexMagazinAmmo` _gun))))

(fn `OnReloadInput`
  (params (`Input Type` :type "/Game/0_Design/ENUM_InputActionType Enum" :default "NewEnumerator0"))
  (if (`self.IsAmmoFull`)
    (`KismetSystemLibrary.PrintText` "FULL AMMO")
    (else
      (switch `/Game/0_Design/ReloadSystem/Enums/EPrimaryGunState` (`self.CurrentGunState`)
        (:`NewEnumerator0`
          (`self.StartReloadSequence`))))))

(fn `UpdateAmmoCount`
  (params (NewCount :type Integer))
  (returns (Output_Get :type Integer))
  (bind _output_get (set `/Game/0_Design/GameManagement_/BP_Gun.IndexMagazinAmmo` NewCount (`self.Gun`)))
  (return _output_get))

(fn `UpdateCurrentReloadState`
  (params (NewState :type "/Game/0_Design/ReloadSystem/Enums/EPrimaryGunReloadState Enum" :default "NewEnumerator0"))
  (bind _output_get (set `self.CurrentReloadState` NewState))
  (switch `/Game/0_Design/ReloadSystem/Enums/EPrimaryGunReloadState` _output_get
    (:`NewEnumerator0`
      (`KismetSystemLibrary.PrintString` "START NORMAL"))
    (:`NewEnumerator1`
      (`KismetSystemLibrary.PrintString` "START FINISHED"))))