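; Player interaction component that targets one of the registered nearby interactables and triggers it on the interact input.
; Add and remove functions maintain the nearby list, which Tick scans only while it is non-empty.
; Selection uses dot products against the deprojected screen-centre ray to favour the interactable most aligned with the view.
; Target changes fire targeted and untargeted calls and refresh the HUD prompt by interaction type.
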(event `self.ReceiveBeginPlay`
  ;[1 0 0.01859 0.25] BEGIN PLAY
  (`KismetSystemLibrary.DelayUntilNextTick`)
  (`self.GetReferences`))

(event `self.ReceiveTick`
  (params (DeltaSeconds :type "Float (single-precision)"))
  ;[1 0 0.01859 0.25] TICK
  (if (`self.bNearInteractables`)
    (`self.GetClosestInteractable`)))

(event `EnhancedInput|/TPS_FeedlingAddon/TPS/_Input/IA_TPS_Interact`
  (params (ActionValue :type Boolean) (ElapsedSeconds :type "Float (double-precision)") (TriggeredSeconds :type "Float (double-precision)") (InputAction :type "InputAction Object Reference" :default "/TPS_FeedlingAddon/TPS/_Input/IA_TPS_Interact.IA_TPS_Interact"))
  ;[1 0 0.01859 0.25] INTERACT
  (:`Started`
    (bind _currentinteractable (`self.CurrentInteractable`)
      (:`then`
        (`/Game/Design/GPE/Old_Interactables/BP_InteractableComponent.OnInteract` _currentinteractable))
      (:`else`))))

(fn `AddNearInteractable`
  (params (Interactable :type "/Game/Design/GPE/Old_Interactables/BP_InteractableComponent Object Reference (by ref)"))
  (`KismetArrayLibrary.Array_AddUnique` (`self.Interactables`) Interactable)
  (set `self.bNearInteractables` true))

(fn `GetClosestInteractable`
  (locals (TargetDirection :type "Vector Structure" :default (0.0 0.0 0.0)) (PlayerLocation :type "Vector Structure" :default (0.0 0.0 0.0)) (ClosestAlignement :type "Float (double-precision)") (ClosestInteractable :type "/Game/Design/GPE/Old_Interactables/BP_InteractableComponent Object Reference"))
  (bind (_worldposition _worlddirection) (`GameplayStatics.DeprojectScreenToWorld` (`self.PlayerController`) (* (`WidgetLayoutLibrary.GetViewportSize`) (0.5 0.5))))
  (bind _returnvalue (`KismetMathLibrary.Dot_VectorVector` (`local.TargetDirection`) _worlddirection))
  (set `local.PlayerLocation` _worldposition)
  (for _array_element (`self.Interactables`)
    (set `local.TargetDirection` (`KismetMathLibrary.Normal` (- (`local.PlayerLocation`) (`Actor.K2_GetActorLocation` (`self.GetOwner` _array_element)))))
    (if (< _returnvalue (`local.ClosestAlignement`))
      (set `local.ClosestAlignement` _returnvalue)
      (set `local.ClosestInteractable` _array_element)))
  (if (!= (`self.CurrentInteractable`) (`local.ClosestInteractable`))
    (bind _currentinteractable (`self.CurrentInteractable`)
      (:`then`
        (`/Game/Design/GPE/Old_Interactables/BP_InteractableComponent.OnUntargeted` _currentinteractable))
      (:`else`
        _))
    (bind _output_get (set `self.CurrentInteractable` (`local.ClosestInteractable`)))
    (if (`KismetSystemLibrary.IsValid` _output_get)
      (`/Game/Design/GPE/Old_Interactables/BP_InteractableComponent.OnTargeted` _output_get)
      (`self.UpdapteViewport`))))

(fn `GetReferences`
  (set `self.PlayerController` (`Pawn.GetLocalViewingPlayerController` (`Actor.Instigator` (`self.GetOwner`)))))

(fn `RemoveNearInteractable`
  (params (Interactable :type "/Game/Design/GPE/Old_Interactables/BP_InteractableComponent Object Reference (by ref)"))
  (bind _interactables (`self.Interactables`))
  (`|ExecutionSequence`
    (:`then_0`
      (`KismetArrayLibrary.Array_RemoveItem` _interactables Interactable)
      (if (`KismetArrayLibrary.Array_IsEmpty` _interactables)
        (set `self.bNearInteractables` false)
        (set `self.CurrentInteractable` null)))
    (:`then_1`
      (`self.UpdapteViewport`))))

(fn `UpdapteViewport`
  (bind _returnvalue (`PlayerController.GetHUD` (`self.PlayerController`)))
  (if (> (`KismetArrayLibrary.Array_Length` (`self.Interactables`)) 0)
    (message `/Game/Design/_GameManagement/BPI_HUD.UpdatePrompts` _returnvalue (`/Game/Design/GPE/Old_Interactables/BP_InteractableComponent.InteractionType` (`self.CurrentInteractable`)))
    (else
      (message `/Game/Design/_GameManagement/BPI_HUD.UpdatePrompts` _returnvalue "DEFAULT"))))