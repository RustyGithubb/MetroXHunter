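; BP_SmartSpawner is a one-shot enemy spawner that waits until the player has looked at its spawn point several times, then spawns while they look away.
; A sphere trigger enables Tick, which uses a view dot product and timers to count sustained looks and time look-aways.
; Enough looks and a long enough look-away spawn a BP_ZeroEnemy or BP_Parasite facing the player, then destroy the spawner.
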(event `self.ReceiveTick`
  (params (DeltaSeconds :type "Float (single-precision)"))
  (bind _player (`self.Player`))
  (if (> (`KismetMathLibrary.Dot_VectorVector` (`KismetMathLibrary.GetForwardVector` (`Pawn.GetControlRotation` _player)) (`KismetMathLibrary.GetDirectionUnitVector` (`self.GetActorEyesViewPoint` _player) (`self.GetWorldSpawnLocation`))) 0.5)
    (if (not (`self.bWasLooking`))
      (set `self.bWasLooking` true)
      (set `self.CurrentLookTime` 0.0)
      (set `self.bHasLooked` false))
    (bind _return (`/Game/Design/Libraries/BPL_GeneralUtilities.Increase Value Float` (`self.CurrentLookTime`) DeltaSeconds))
    (if (and (>= _return (`self.MinLookTime`)) (not (`self.bHasLooked`)))
      (`/Engine/EditorBlueprintResources/StandardMacros.IncrementInt` (`self.LookedTimes`)
        (:`  `
          (set `self.bHasLooked` true))))
    (else
      (if (`self.bWasLooking`)
        (set `self.bWasLooking` false)
        (set `self.CurrentLookTime` 0.0))
      (bind _return_2 (`/Game/Design/Libraries/BPL_GeneralUtilities.Increase Value Float` (`self.CurrentLookTime`) DeltaSeconds))
      (if (>= _return_2 (`self.MinUnLookTime`))
        (if (>= (`self.LookedTimes`) (`self.RequiredLookedTimesToSpawn`))
          (`self.SpawnEnemy`))))))

(event `self.SphereOverlap.OnComponentBeginOverlap`
  (params (OverlappedComponent :type "PrimitiveComponent Object Reference") (OtherActor :type "Actor Object Reference") (OtherComp :type "PrimitiveComponent Object Reference") (OtherBodyIndex :type Integer) (bFromSweep :type Boolean) (SweepResult :type "HitResult Structure (by ref)"))
  (bind _ascharacter (cast `Character` OtherActor))
  (`self.SetActorTickEnabled` true)
  (set `self.Player` _ascharacter))

(event `self.SphereOverlap.OnComponentEndOverlap`
  (params (OverlappedComponent :type "PrimitiveComponent Object Reference") (OtherActor :type "Actor Object Reference") (OtherComp :type "PrimitiveComponent Object Reference") (OtherBodyIndex :type Integer))
  (`self.SetActorTickEnabled` false)
  (set `self.Player` null))

(fn `GetWorldSpawnLocation`
  (returns (ReturnValue :type "Vector Structure"))
  (return (`KismetMathLibrary.TransformLocation` (`self.GetTransform`) (`self.SpawnPosition`))))

(fn `SpawnEnemy`
  (bind _returnvalue (`self.GetWorldSpawnLocation`))
  (bind _returnvalue_2 (`KismetMathLibrary.Conv_VectorToRotator` (`KismetMathLibrary.GetDirectionUnitVector` (`self.GetWorldSpawnLocation`) (`self.K2_GetActorLocation` (`self.Player`)))))
  (if (`self.bSpawnZeroEnemy`)
    (`|SpawnActorFromClass` "/Game/Design/Enemies/AI/Zero/BP_ZeroEnemy.BP_ZeroEnemy_C" (`KismetMathLibrary.MakeTransform` _returnvalue _returnvalue_2) "AdjustIfPossibleButAlwaysSpawn" "MultiplyWithRoot" null (`self.SpawnDataAsset`) null)
    (else
      (`|SpawnActorFromClass` "/Game/Design/Enemies/AI/Parasite/BP_Parasite.BP_Parasite_C" (`KismetMathLibrary.MakeTransform` _returnvalue _returnvalue_2) "AdjustIfPossibleButAlwaysSpawn" "MultiplyWithRoot" null null)))
  (`self.K2_DestroyActor`))

(fn `UserConstructionScript`
  (bind _spawnposition (`self.SpawnPosition`))
  (`SphereComponent.SetSphereRadius` (`self.SphereOverlap`) (`self.TriggerRadius`) false)
  (`SceneComponent.K2_SetRelativeLocation` (`self.SpawnBillboard`) _spawnposition false false)
  (`KismetSystemLibrary.DrawDebugBox` (+ (`self.K2_GetActorLocation`) _spawnposition) (60.0 60.0 60.0) (struct :`R` 1.0 :`A` 1.0) (struct) 0.0 16.0))