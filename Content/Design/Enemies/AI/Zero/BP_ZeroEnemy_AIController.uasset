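; AI controller Blueprint for the Zero enemy, holding event logic for stun reactions and attack reservations, though none of it is hooked up in this graph.
; The stun handler drops Rush Attack or Melee Attack back to Chase, and the substate handler frees AttackerComponent reservations, a job now noted as handled by Behavior Tree services.
; Possess is empty, and both the handler bindings and the player auto-targeting are disconnected.
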(event `self.ReceivePossess`
  (params (PossessedPawn :type "Pawn Object Reference")))

(event `OnPawnStun`
  ;[0 0 0 0.33] DOP: Change state when stun
  (switch `EZeroEnemyAIState` (`self.GetState`)
    (:`RushAttack`
      _)
    (:`MeleeAttack`
      _))
  (`self.SetState` "Chase"))

(event `OnSubstateSwitched_Event`
  ;[0 0 0 0.33] DOP: Free AI reservations on substate change;
  ; Now, managed through BT's services
  (`AIAttackerComponent.FreeReservations` (`self.AttackerComponent`)))

(fn `UserConstructionScript`)