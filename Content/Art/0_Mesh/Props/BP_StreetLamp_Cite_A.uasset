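; Street lamp prop with three bulbs that takes part in a light-flicker system.
; It offers the spot lights enabled in LightsON as flickable; flicker start swaps those bulbs to a test material and sets a base intensity.
; Flicker stop restores materials cached at BeginPlay and zeroes all three numbered spot lights; tick and update hooks are empty.
; A bulb-destroyed counter removes the SpotLight component and stops audio when none remain.
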(event `self.ReceiveBeginPlay`
  (`KismetArrayLibrary.Array_Add` (`self.Materials`) (`PrimitiveComponent.GetMaterial` (`self.Bulb_0`) 0))
  (`KismetArrayLibrary.Array_Add` (`self.Materials`) (`PrimitiveComponent.GetMaterial` (`self.Bulb_1`) 0))
  (`KismetArrayLibrary.Array_Add` (`self.Materials`) (`PrimitiveComponent.GetMaterial` (`self.Bulb_2`) 0)))

(event `OnBulbDestroyed`
  (bind _result (`/Engine/EditorBlueprintResources/StandardMacros.DecrementInt` (`self.LightBulbLeft`))
    (:`  `
      (if (== _result 0)
        (`ActorComponent.K2_DestroyComponent` (`self.SpotLight`))
        (`AudioComponent.Stop` (`self.Audio`))))))

(fn `OnFlickLightStart`
  (params (LightData :type "LightData Structure (by ref)"))
  (`|ExecutionSequence`
    (:`then_0`
      (if (`|GetArrayItem` (`self.LightsON`))
        (`PrimitiveComponent.SetMaterial` (`self.Bulb_0`) 0 "/Game/Design/GPE/Destructible/Lights/MI_BulbTEST.MI_BulbTEST")))
    (:`then_1`
      (if (`|GetArrayItem` (`self.LightsON`) 1)
        (`PrimitiveComponent.SetMaterial` (`self.Bulb_1`) 0 "/Game/Design/GPE/Destructible/Lights/MI_BulbTEST.MI_BulbTEST")))
    (:`then_2`
      (if (`|GetArrayItem` (`self.LightsON`) 2)
        (`PrimitiveComponent.SetMaterial` (`self.Bulb_2`) 0 "/Game/Design/GPE/Destructible/Lights/MI_BulbTEST.MI_BulbTEST")))
    (:`then_3`
      (setmembers `LightData` :`StructRef` LightData :`OriginalLightIntensity` 5000.0))))

(fn `OnFlickLightStop`
  (params (LightData :type "LightData Structure (by ref)"))
  (`|ExecutionSequence`
    (:`then_0`
      (`PrimitiveComponent.SetMaterial` (`self.Bulb_0`) 0 (`|GetArrayItem` (`self.Materials`))))
    (:`then_1`
      (`PrimitiveComponent.SetMaterial` (`self.Bulb_1`) 0 (`|GetArrayItem` (`self.Materials`) 1)))
    (:`then_2`
      (`PrimitiveComponent.SetMaterial` (`self.Bulb_2`) 0 (`|GetArrayItem` (`self.Materials`) 2)))
    (:`then_3`
      (`LightComponent.SetIntensity` (`self.SpotLight_0`) 0.0)
      (`LightComponent.SetIntensity` (`self.SpotLight_1`) 0.0)
      (`LightComponent.SetIntensity` (`self.SpotLight_2`) 0.0)
      (return))))

(fn `OnFlickLightTick`
  (params (DeltaTime :type "Float (single-precision)") (LightData :type "LightData Structure (by ref)"))
  (return))

(fn `OnFlickLightUpdate`
  (params (LightData :type "LightData Structure (by ref)") (IntensityScale :type "Float (single-precision)"))
  (return))

(fn `RetrieveFlickableLights`
  (returns (ReturnValue :type "Array of LightComponent Object Reference"))
  (locals (FlickableLights :type "Array of LightComponent Object Reference"))
  (`|ExecutionSequence`
    (:`then_0`
      (if (`|GetArrayItem` (`self.LightsON`))
        (`KismetArrayLibrary.Array_Add` (`local.FlickableLights`) (`self.SpotLight_0`))))
    (:`then_1`
      (if (`|GetArrayItem` (`self.LightsON`) 1)
        (`KismetArrayLibrary.Array_Add` (`local.FlickableLights`) (`self.SpotLight_1`))))
    (:`then_2`
      (if (`|GetArrayItem` (`self.LightsON`) 2)
        (`KismetArrayLibrary.Array_Add` (`local.FlickableLights`) (`self.SpotLight_2`))))
    (:`then_3`
      (return (`local.FlickableLights`)))))

(fn `UserConstructionScript`)