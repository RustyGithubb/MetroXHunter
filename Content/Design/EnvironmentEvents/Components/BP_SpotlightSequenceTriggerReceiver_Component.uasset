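; Trigger receiver component that switches on the lights of assigned actors one actor at a time, as a timed spotlight sequence.
; On BeginPlay it caches every light component and its scene intensity in flattened arrays with per-actor last indices, then dims them to zero.
; The trigger event starts a self-recalling delayed loop that restores each actor's intensities, first-to-last or reversed.
; Missing actors or lights print setup errors.
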(event `self.ReceiveBeginPlay`
  (if (`KismetArrayLibrary.Array_IsNotEmpty` (`self.ActorsToTurnOn`))
    (`self.RegisterAllLights`)
    ;[1 1 1 0.33] They should be lit up, so they start off!
    (for _array_element (`self.LightsToChange`)
      (`LightComponent.SetIntensity` _array_element 0.0))
    (else
      ;[0.0625 0.001432 0 0.33] ERROR PRINT
      (`KismetSystemLibrary.PrintText` (`|FormatText` "SpotlightSequenceComponent on Actor {actorName} \nhas not been given Actors to change. \nPlease Add one." (`KismetSystemLibrary.GetDisplayName` (`self.GetOwner`))) true true (struct :`R` 1.0 :`A` 1.0) 500.0))))

(event `StartSequence`
  (if (`self.TurnOnFirstToLast`)
    (set `self.CurrentLightIndex` 0)
    (set `self.CurrentActorIndex` 0)
    (`self.NextForwardSequence`)
    (else
      (set `self.CurrentLightIndex` (`KismetArrayLibrary.Array_LastIndex` (`self.LightsToChange`)))
      (set `self.CurrentActorIndex` (`KismetArrayLibrary.Array_LastIndex` (`self.ActorsToTurnOn`)))
      (`self.NextBackwardSequence`))))

(event `NextForwardSequence`
  (bind _currentlightindex (`self.CurrentLightIndex`))
  ;[1 1 1] Do the lights for the current Actor
  (for _ (range (+ (`|GetArrayItem` (`self.LightsPerActor`) (`self.CurrentActorIndex`)) 1))
    (`LightComponent.SetIntensity` (`|GetArrayItem` (`self.LightsToChange`) _currentlightindex) (`|GetArrayItem` (`self.LightsTargetIntensity`) _currentlightindex))
    (`/Engine/EditorBlueprintResources/StandardMacros.IncrementInt` (`self.CurrentLightIndex`)))
  (bind _result (`/Engine/EditorBlueprintResources/StandardMacros.IncrementInt` (`self.CurrentActorIndex`))
    (:`  `
      (if (<= _result (`KismetArrayLibrary.Array_LastIndex` (`self.ActorsToTurnOn`)))
        (`KismetSystemLibrary.Delay` (`self.DelayBetweenLights`))
        (`self.NextForwardSequence`)))))

(event `NextBackwardSequence`
  (bind _currentlightindex (`self.CurrentLightIndex`))
  ;[1 1 1] Do the lights for the current Actor
  (for _ (range (+ (`|GetArrayItem` (`self.LightsPerActor`) (`self.CurrentActorIndex`)) 1))
    (`LightComponent.SetIntensity` (`|GetArrayItem` (`self.LightsToChange`) _currentlightindex) (`|GetArrayItem` (`self.LightsTargetIntensity`) _currentlightindex))
    (`/Engine/EditorBlueprintResources/StandardMacros.DecrementInt` (`self.CurrentLightIndex`)))
  (bind _result (`/Engine/EditorBlueprintResources/StandardMacros.DecrementInt` (`self.CurrentActorIndex`))
    (:`  `
      (if (>= _result 0)
        (`KismetSystemLibrary.Delay` (`self.DelayBetweenLights`))
        (`self.NextBackwardSequence`)))))

(fn `OnPlayComponentSpecificEvent`
  (params (FromBoxEnter :type Boolean) (TriggerBox :type "Actor Object Reference"))
  (`self.StartSequence`))

(fn `RegisterAllLights`
  (locals (CurrentlyEvaluatedLights :type "Array of LightComponent Object Reference"))
  (`KismetArrayLibrary.Array_Clear` (`self.LightsTargetIntensity`))
  (`KismetArrayLibrary.Array_Clear` (`self.LightsToChange`))
  (`KismetArrayLibrary.Array_Clear` (`self.LightsPerActor`))
  ;[0.1724 0.05414 0.1771 0.33] Loop through all given Actors and get all of their Lights (if they have any!!)
  (for _array_element (`self.ActorsToTurnOn`)
    (bind _output_get (set `local.CurrentlyEvaluatedLights` (`Actor.K2_GetComponentsByClass` _array_element "/Script/Engine.LightComponent")))
    (if (`KismetArrayLibrary.Array_IsNotEmpty` _output_get)
      (`KismetArrayLibrary.Array_Add` (`self.LightsPerActor`) (`KismetArrayLibrary.Array_LastIndex` _output_get))
      ;[0.1979 0.08918 0.04725 0.33] Register each Light with their Starting Intensity (which the intensity in the scene)
      (for _array_element_2 (`local.CurrentlyEvaluatedLights`)
        (`KismetArrayLibrary.Array_Add` (`self.LightsToChange`) _array_element_2)
        (`KismetArrayLibrary.Array_Add` (`self.LightsTargetIntensity`) (`LightComponentBase.Intensity` _array_element_2)))
      (else
        ;[0.1927 0 0 0.33] ERROR PRINT
        (`KismetSystemLibrary.PrintText` (`|FormatText` "SpotlightSequenceComponent on Actor {actorName} \nhas been given Actor {fakeLight}, but it doesn't have any Light Components. \nPlease remove the Actor or add a Light to it." (`KismetSystemLibrary.GetDisplayName` (`self.GetOwner`)) (`KismetSystemLibrary.GetDisplayName` _array_element)) true true (struct :`R` 1.0 :`A` 1.0) 500.0)))))