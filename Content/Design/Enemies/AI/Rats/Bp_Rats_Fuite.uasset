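; Fleeing rat enemy that runs away from the player, squeaks at random intervals and destroys itself after 20 seconds.
; Tick eases its heading away from the player, adds sideways weaving from a curve over time, and feeds speed into a dynamic material's Velocity parameter.
; On death it unlocks the RATATOUILLE_2 achievement, then METRO once the GameInstance count reaches all normal achievements.
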(event `self.ReceiveBeginPlay`
  (bind _staticmesh (`self.StaticMesh`))
  ;[1 0 0 0.33] BEGIN PLAY
  (`|ExecutionSequence`
    (:`then_0`
      (bind _returnvalue (`PrimitiveComponent.CreateDynamicMaterialInstance` _staticmesh 0 (`PrimitiveComponent.GetMaterial` _staticmesh 0) "None"))
      (`self.OnAudioFinished_Event`)
      (add `AudioComponent.OnAudioFinished` (`self.Audio`) (delegate `OnAudioFinished_Event`))
      (`KismetSystemLibrary.Delay` 20.0)
      (`self.K2_DestroyActor`))
    (:`then_1`
      (set `self.Current` (`self.GetActorForwardVector`)))
    (:`then_2`
      (bind _asbp_metro_game_instance (cast `/Game/Design/_GameManagement/Core/BP_MetroGameInstance` (`GameplayStatics.GetGameInstance`)))
      (set `self.Game Instance` _asbp_metro_game_instance))))

(event `OnAudioFinished_Event`
  ;[1 0 0 0.33] BEGIN PLAY
  (`KismetSystemLibrary.Delay` (`KismetMathLibrary.RandomFloatInRange` 0.5 3.0))
  (`AudioComponent.Play` (`self.Audio`) 0.0))

(event `self.ReceiveTick`
  (params (DeltaSeconds :type "Float (single-precision)"))
  (set `self.Time Duration` (+ (`self.Time Duration`) DeltaSeconds 0.0))
  (`/Engine/EditorBlueprintResources/StandardMacros.IsValid` (stale `self.ReceiveBeginPlay` _returnvalue)
    (:`Is Valid`
      (`MaterialInstanceDynamic.SetScalarParameterValue` (stale `self.ReceiveBeginPlay` _returnvalue) "Velocity" (* (`KismetMathLibrary.VSize` (`self.GetVelocity`)) 1.0))
      (bind _output_get (set `self.Current` (`KismetMathLibrary.VInterpTo` (`self.Current`) (* (`KismetMathLibrary.GetDirectionUnitVector` (`self.K2_GetActorLocation`) (`self.K2_GetActorLocation` (`GameplayStatics.GetPlayerCharacter` 0))) -10.0) (`GameplayStatics.GetWorldDeltaSeconds`) 0.1)))
      (`self.AddMovementInput` _output_get)
      (`self.AddMovementInput` (`self.GetActorRightVector`) (`CurveFloat.GetFloatValue` (`self.Curve`) (`self.Time Duration`))))))

(event `self.Health.OnDeath`
  (params (DamageContext :type "DamageContext Structure (by ref)"))
  (bind _returnvalue (`GameplayStatics.GetPlayerController` 0))
  (bind _returnvalue_2 (`GameplayStatics.GetPlayerController` 0))
  (bind _game_instance (`self.Game Instance`))
  ;[1 0 0 0.33] DESTROY
  ;[0 1 0.8336 0.33] ACHIEVEMENT : RATATOUILLE_2
  (`AchievementQueryCallbackProxy.CacheAchievements` _returnvalue
    (:`OnSuccess`
      (bind (_bfoundid _progress) (`AchievementBlueprintLibrary.GetCachedAchievementProgress` _returnvalue "RATATOUILLE_2"))
      (if _bfoundid
        (if (> _progress 0.0)
          (`KismetSystemLibrary.PrintString` "Achievements already unlocked !" true true (struct :`G` 1.0 :`B` 0.012183 :`A` 1.0) 6.0)
          (`self.K2_DestroyActor` :!label _label)
          (else
            (`AchievementWriteCallbackProxy.WriteAchievementProgress` _returnvalue "RATATOUILLE_2"
              (:`OnSuccess`
                (`|ExecutionSequence`
                  (:`then_0`
                    (goto _label))
                  (:`then_1`
                    (`KismetSystemLibrary.PrintString` "Achievement unlocked !" true true (struct :`G` 1.0 :`B` 0.96591 :`A` 1.0) 6.0)
                    (set `/Game/Design/_GameManagement/Core/BP_MetroGameInstance.AchievementsUnlocked` (+ (`/Game/Design/_GameManagement/Core/BP_MetroGameInstance.AchievementsUnlocked` _game_instance) 1) _game_instance)
                    (if (== (`/Game/Design/_GameManagement/Core/BP_MetroGameInstance.AchievementsUnlocked` _game_instance) (`/Game/Design/_GameManagement/Core/BP_MetroGameInstance.TotalNormalAchievements` _game_instance))
                      (bind (_bfoundid_2 _progress_2) (`AchievementBlueprintLibrary.GetCachedAchievementProgress` _returnvalue_2 "METRO"))
                      (if _bfoundid_2
                        (if (> _progress_2 0.0)
                          (`KismetSystemLibrary.PrintString` "Achievements already unlocked !" true true (struct :`G` 1.0 :`B` 0.012183 :`A` 1.0) 10.0)
                          (else
                            (`AchievementWriteCallbackProxy.WriteAchievementProgress` _returnvalue_2 "METRO")))
                        (else
                          (`KismetSystemLibrary.PrintString` "Didn't find ID" true true (struct :`R` 1.0 :`G` 0.408724 :`A` 1.0) 10.0))))))))))
        (else
          (`KismetSystemLibrary.PrintString` "Didn't find ID" true true (struct :`R` 1.0 :`G` 0.408724 :`A` 1.0) 6.0))))
    (:`OnFailure`
      (`KismetSystemLibrary.PrintString` "Couldn't cache achievements !" true true (struct :`R` 1.0 :`A` 1.0) 6.0))))

(fn `UserConstructionScript`)