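; Cheat function that teleports the controlled pawn to a selected PlayerStart in the level, matching its rotation on both the pawn and the camera.
; On init and on each streamed level load, it gathers all PlayerStarts and builds option names from their tags, adding numeric suffixes to duplicates.
; A changed selection is only recorded; teleporting requires triggering the same index again, so cycling through options does not move the player.
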(event `self.OnInit`
  (add `MetroXHunterGameInstance.OnLevelStreamingLoad` (cast `MetroXHunterGameInstance` (`GameplayStatics.GetGameInstance`) :!pure true) (delegate `OnLevelStreamingLoad_Event`))
  ;[1 1 1 0.33] Find all PlayerStarts
  (bind _outactors (`GameplayStatics.GetAllActorsOfClass` "/Script/Engine.PlayerStart" :!label _label))
  (bind _output_get (set `self.PlayerStartActors` _outactors))
  (`KismetArrayLibrary.Array_Clear` (`self.ValueNames`))
  (for _array_element _output_get
    (bind _uniquevaluename (`self.FindUniqueValueName` (`KismetStringLibrary.Conv_NameToString` (`PlayerStart.PlayerStartTag` _array_element))))
    (`KismetArrayLibrary.Array_Add` (`self.ValueNames`) _uniquevaluename)))

(event `OnLevelStreamingLoad_Event`
  (params (LevelName :type Name))
  (goto _label))

(event `self.OnCheat`
  (bind _index (`self.Index`))
  (bind _returnvalue (`CheatManager.GetPlayerController` (`self.CheatManager`)))
  (bind _output (`|GetArrayItem` (`self.PlayerStartActors`) _index))
  (bind _returnvalue_2 (`Actor.K2_GetActorRotation` _output))
  (if (`KismetArrayLibrary.Array_IsNotEmpty` (`self.PlayerStartActors`))
    ;[1 1 1 0.33] Avoid spawn when cycling through elements
    (if (== (`self.Index`) (`self.LastIndex`))
      (`Actor.K2_SetActorLocationAndRotation` (`Controller.K2_GetPawn` _returnvalue) (`Actor.K2_GetActorLocation` _output) _returnvalue_2 false true)
      (`Controller.SetControlRotation` _returnvalue _returnvalue_2) ; Update the camera rotation
      (`KismetSystemLibrary.PrintText` (`|FormatText` "CheatFunction: Teleported to {ValueName}" (`|GetArrayItem` (`self.ValueNames`) _index)))
      (else
        (set `self.LastIndex` (`self.Index`))))))

(fn `FindUniqueValueName`
  (params (ValueName :type String))
  (returns (UniqueValueName :type String))
  (locals (NewValueName :type String) (MaxIterations :type Integer :default 32))
  (bind _newvaluename (`local.NewValueName`))
  (bind _maxiterations (`local.MaxIterations`))
  (set `local.NewValueName` ValueName)
  ;[1 1 1 0.33] Ensure uniqueness of the name by iterating through a range of numbers
  (for _index (range (+ _maxiterations 1))
    (if (`KismetArrayLibrary.Array_Contains` (`self.ValueNames`) _newvaluename)
      (set `local.NewValueName` (`KismetStringLibrary.Concat_StrStr` ValueName (`KismetStringLibrary.Conv_IntToString` (+ _index 1))))
      (else
        (return _newvaluename))))
  ;[1 0 0 0.33] Fail: Maximum iterations has been reached
  (`KismetSystemLibrary.PrintText` (`|FormatText` "CheatFunction_TeleportTo: Couldn't find an unique value name for {ValueName} after maximum iterations of {MaxIterations}!" ValueName _maxiterations) true true (struct :`R` 1.0 :`A` 1.0) 5.0)
  (return ValueName))