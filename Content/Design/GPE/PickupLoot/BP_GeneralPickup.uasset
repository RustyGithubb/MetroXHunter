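; General world pickup for loot such as ammo or syringe liquid, collected into the player's inventory on interaction.
; An outer overlap shows its interaction widget, while an inner overlap registers it as a nearby interactable and caches the character's inventory component.
; Targeting events update the widget, whose sprite is set from the pickup type at BeginPlay.
; Interacting keeps the amount AddToInventory returns, destroying the pickup when it reaches zero.
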(event `self.ReceiveBeginPlay`
  (bind _aswbp_interactable (cast `/Game/Design/Widgets/WBP_Interactable` (`WidgetComponent.GetWidget` (`self.Widget`))))
  (set `self.InteractableWidget` _aswbp_interactable)
  (`self.EditSprite`))

(event `self.InteractableComponent.OnInteract`
  (bind _interactablecomponent (`self.InteractableComponent`))
  ;[1 1 1 0.33] INTERACT
  (bind _overflow (`/Game/Design/_GameManagement/BP_InventoryComponent.AddToInventory` (`self.PlayerInventory`) (`self.PickupType`) (`self.Amount`)))
  (bind _output_get (set `self.Amount` _overflow))
  (if (== _output_get 0)
    (bind _playerinteractioncomponent (`/Game/Design/GPE/Old_Interactables/BP_InteractableComponent.PlayerInteractionComponent` _interactablecomponent)
      (:`then`
        (`/Game/Design/GPE/Old_Interactables/BP_InteractionComponent.RemoveNearInteractable` _playerinteractioncomponent _interactablecomponent)
        (`self.K2_DestroyActor`))
      (:`else`))))

(event `self.InnerInteraction.OnComponentBeginOverlap`
  (params (OverlappedComponent :type "PrimitiveComponent Object Reference") (OtherActor :type "Actor Object Reference") (OtherComp :type "PrimitiveComponent Object Reference") (OtherBodyIndex :type Integer) (bFromSweep :type Boolean) (SweepResult :type "HitResult Structure (by ref)"))
  (bind _returnvalue (`self.GetComponentByClass` OtherActor "/Game/Design/_GameManagement/BP_InventoryComponent.BP_InventoryComponent_C"))
  ;[1 1 1 0.33] OVERLAP INNER CIRCLE
  (cast `Character` OtherActor)
  (`/Game/Design/GPE/Old_Interactables/BP_InteractableComponent.AddNearInteractable` (`self.InteractableComponent`) OtherActor)
  (`/Engine/EditorBlueprintResources/StandardMacros.IsValid` _returnvalue
    (:`Is Valid`
      (set `self.PlayerInventory` _returnvalue))))

(event `self.InnerInteraction.OnComponentEndOverlap`
  (params (OverlappedComponent :type "PrimitiveComponent Object Reference") (OtherActor :type "Actor Object Reference") (OtherComp :type "PrimitiveComponent Object Reference") (OtherBodyIndex :type Integer))
  ;[1 1 1 0.33] END OVERLAP INNER CIRCLE
  (cast `Character` OtherActor)
  (`/Game/Design/GPE/Old_Interactables/BP_InteractableComponent.RemoveNearInteractable` (`self.InteractableComponent`))
  (`/Game/Design/Widgets/WBP_Interactable.OnUntargeted` (`self.InteractableWidget`)))

(event `self.OutterInteraction.OnComponentBeginOverlap`
  (params (OverlappedComponent :type "PrimitiveComponent Object Reference") (OtherActor :type "Actor Object Reference") (OtherComp :type "PrimitiveComponent Object Reference") (OtherBodyIndex :type Integer) (bFromSweep :type Boolean) (SweepResult :type "HitResult Structure (by ref)"))
  ;[1 1 1 0.33] OVERLAP OUTTER CIRCLE
  (cast `Character` OtherActor)
  (`SceneComponent.SetHiddenInGame` (`self.Widget`) false false))

(event `self.OutterInteraction.OnComponentEndOverlap`
  (params (OverlappedComponent :type "PrimitiveComponent Object Reference") (OtherActor :type "Actor Object Reference") (OtherComp :type "PrimitiveComponent Object Reference") (OtherBodyIndex :type Integer))
  ;[1 1 1 0.33] END OVERLAP OUTTER CIRCLE
  (cast `Character` OtherActor)
  (`SceneComponent.SetHiddenInGame` (`self.Widget`) true false))

(event `self.InteractableComponent.OnTargeted`
  ;[1 1 1 0.33] ON TARGETED
  (`/Game/Design/Widgets/WBP_Interactable.OnTargeted` (`self.InteractableWidget`) (`self.Amount`)))

(event `self.InteractableComponent.OnUntargeted`
  ;[1 1 1 0.33] ON UNTARGETED
  (`/Game/Design/Widgets/WBP_Interactable.OnUntargeted` (`self.InteractableWidget`)))

(fn `EditSprite`
  (bind _sprite (`/Game/Design/Widgets/WBP_Interactable.Sprite` (`self.InteractableWidget`)))
  (switch `/Game/Design/GPE/PickupLoot/E_PickupType` (`self.PickupType`)
    (:`NewEnumerator0`
      (`Image.SetBrush` _sprite (make `SlateBrush` "Image" "NoTile" "NoMirror" (make `DeprecateSlateVector2D` 50.0 50.0) (struct) (struct :`SpecifiedColor` (struct :`R` 1.0 :`G` 1.0 :`B` 1.0 :`A` 1.0) :`ColorUseRule` "UseColor_Specified") (struct :`CornerRadii` (struct) :`Color` (struct :`SpecifiedColor` (struct) :`ColorUseRule` "UseColor_Specified") :`RoundingType` "HalfHeightRadius") "/Game/Art/UI/Sprites/Placeholder/ammo_Sprite.ammo_Sprite")))
    (:`NewEnumerator1`
      (`Image.SetBrush` _sprite (make `SlateBrush` "Image" "NoTile" "NoMirror" (make `DeprecateSlateVector2D` 50.0 50.0) (struct) (struct :`SpecifiedColor` (struct :`R` 1.0 :`G` 1.0 :`B` 1.0 :`A` 1.0) :`ColorUseRule` "UseColor_Specified") (struct :`CornerRadii` (struct) :`Color` (struct :`SpecifiedColor` (struct) :`ColorUseRule` "UseColor_Specified") :`RoundingType` "HalfHeightRadius") "/Game/Art/UI/Sprites/Placeholder/Doctor-Needle-PNG-Clipart_Sprite.Doctor-Needle-PNG-Clipart_Sprite")))))

(fn `UserConstructionScript`)