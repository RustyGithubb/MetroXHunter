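; BP_PipeBig is a construction-script tool that builds a large pipe along an editable spline.
; It deforms spline meshes between points and places joint rings at fixed distance intervals, aligned to the tangent.
; Every few rings it spawns four wall-support candidates rotated 90 degrees apart around the pipe axis.
; Supports survive only where they overlap WorldStatic geometry, ignoring blacklisted actors, so the pipe attaches to nearby surfaces automatically.
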(fn `UserConstructionScript`
  (bind _spline (`self.Spline`))
  (bind _spline_2 (`self.Spline`))
  (bind _segmentlenght (`self.SegmentLenght`))
  (for _index (range (`SplineComponent.GetNumberOfSplinePoints` _spline_2))
    (bind _returnvalue (`AddComponent|NODE_AddSplineMeshComponent-0`))
    (`StaticMeshComponent.SetStaticMesh` _returnvalue (`self.Spline Mesh`))
    (`SplineMeshComponent.SetForwardAxis` _returnvalue "X" true)
    (bind _returnvalue_2 (+ _index 1))
    (`SplineMeshComponent.SetStartAndEnd` _returnvalue (`SplineComponent.GetLocationAtSplinePoint` _spline_2 _index "Local") (`SplineComponent.GetTangentAtSplinePoint` _spline_2 _index "Local") (`SplineComponent.GetLocationAtSplinePoint` _spline_2 _returnvalue_2 "Local") (`SplineComponent.GetTangentAtSplinePoint` _spline_2 _returnvalue_2 "Local") true))
  ;[1 1 1 0.33] Rings
  (for _index_2 (range (`.ReturnValue` (`KismetMathLibrary.FMod` (`SplineComponent.GetSplineLength` (`self.Spline`)) _segmentlenght)))
    (bind _returnvalue_3 (`AddComponent|NODE_AddStaticMeshComponent-12`))
    (`StaticMeshComponent.SetStaticMesh` _returnvalue_3 (`self.Raccord Static Mesh`))
    (bind _returnvalue_4 (* _index_2 _segmentlenght))
    (bind _returnvalue_5 (`SplineComponent.GetLocationAtDistanceAlongSpline` _spline _returnvalue_4 "Local"))
    (bind _returnvalue_6 (`SplineComponent.GetTangentAtDistanceAlongSpline` _spline _returnvalue_4 "Local"))
    (`SceneComponent.K2_SetRelativeLocationAndRotation` _returnvalue_3 _returnvalue_5 (`KismetMathLibrary.Conv_VectorToRotator` _returnvalue_6) false false)
    ;[1 1 1 0.33] Supports
    (if (== (`KismetMathLibrary.FMod` (`KismetMathLibrary.Conv_IntToDouble` _index_2) (`KismetMathLibrary.Conv_IntToDouble` (`self.PillarEveryNumberOfRings`))) 0.0)
      (for _index_3 (range 4)
        (bind _returnvalue_7 (`AddComponent|NODE_AddStaticMeshComponent-13`))
        (`StaticMeshComponent.SetStaticMesh` _returnvalue_7 (`self.Wall Accroche Mesh`))
        (`SceneComponent.K2_SetRelativeLocationAndRotation` _returnvalue_7 _returnvalue_5 (`KismetMathLibrary.RotatorFromAxisAndAngle` _returnvalue_6 (* (`KismetMathLibrary.Conv_IntToDouble` _index_3) 90)) false false)
        (bind (_outactors _returnvalue_8) (`KismetSystemLibrary.ComponentOverlapActors` _returnvalue_7 (`SceneComponent.K2_GetComponentToWorld` _returnvalue_7) (`|MakeArray` "ObjectTypeQuery1" :!type "EObjectTypeQuery Enum") null (`self.ConnectionBlackList`)))
        (if (not _returnvalue_8)
          (`ActorComponent.K2_DestroyComponent` _returnvalue_7))))))