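; Trigger receiver component that ignites the lights on assigned actors, fading them up from dark when its trigger event plays.
; At BeginPlay it records each light component's placed intensity as the target, zeroes it, and prints errors for missing actors or lights.
; Tick, enabled only during the transition, scales intensities along a float curve over TransitionTime, then snaps to the targets.
; A zero TransitionTime switches the lights on instantly.
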(event `self.ReceiveBeginPlay`
  (`self.SetComponentTickEnabled` false)
  (if (`KismetArrayLibrary.Array_IsNotEmpty` (`self.ActorsThatShouldChange`))
    (`self.RegisterAllLights`)
    ;[1 1 1 0.33] They should be lit up, so they start off!
    (for _array_element (`self.LightsToChange`)
      (`LightComponent.SetIntensity` _array_element 0.0))
    (else
      ;[0.0625 0.001432 0 0.33] ERROR PRINT
      (`KismetSystemLibrary.PrintText` (`|FormatText` "LightIgniterComponent on Actor {actorName} \nhas not been given Actors to change. \nPlease Add one." (`KismetSystemLibrary.GetDisplayName` (`self.GetOwner`))) true true (struct :`R` 1.0 :`A` 1.0) 500.0))))

(event `self.ReceiveTick`
  (params (DeltaSeconds :type "Float (single-precision)"))
  (bind _return (`/Game/Design/Libraries/BPL_GeneralUtilities.Increase Value Float` (`self.CurrentChangeTime`) (* (`GameplayStatics.GetWorldDeltaSeconds`) (`GameplayStatics.GetGlobalTimeDilation`))))
  (if (>= _return (`self.TransitionTime`))
    (`self.StopLightIgnition`)
    (else
      (`self.UpdateAllLights`))))

(fn `OnPlayComponentSpecificEvent`
  (params (FromBoxEnter :type Boolean) (TriggerBox :type "Actor Object Reference"))
  ;[1 1 1] No need to do the ticks and stuff if you want an instant turn on!
  (if (!= (`self.TransitionTime`) 0.0)
    (`self.SetComponentTickEnabled` true)
    (else
      (for (_array_element _array_index) (`self.LightsToChange`)
        (`LightComponent.SetIntensity` _array_element (`|GetArrayItem` (`self.LightsTargetIntensity`) _array_index))))))

(fn `RegisterAllLights`
  (locals (CurrentlyEvaluatedLights :type "Array of LightComponent Object Reference"))
  (`KismetArrayLibrary.Array_Clear` (`self.LightsTargetIntensity`))
  (`KismetArrayLibrary.Array_Clear` (`self.LightsToChange`))
  ;[0.1724 0.05414 0.1771 0.33] Loop through all given Actors and get all of their Lights (if they have any!!)
  (for _array_element (`self.ActorsThatShouldChange`)
    (bind _output_get (set `local.CurrentlyEvaluatedLights` (`Actor.K2_GetComponentsByClass` _array_element "/Script/Engine.LightComponent")))
    (if (`KismetArrayLibrary.Array_IsNotEmpty` _output_get)
      ;[0.1979 0.08918 0.04725 0.33] Register each Light with their Starting Intensity (which the intensity in the scene)
      (for _array_element_2 (`local.CurrentlyEvaluatedLights`)
        (`KismetArrayLibrary.Array_Add` (`self.LightsToChange`) _array_element_2)
        (`KismetArrayLibrary.Array_Add` (`self.LightsTargetIntensity`) (`LightComponentBase.Intensity` _array_element_2)))
      (else
        ;[0.1927 0 0 0.33] ERROR PRINT
        (`KismetSystemLibrary.PrintText` (`|FormatText` "LightColorChangerComponent on Actor {actorName} \nhas been given Actor {fakeLight}, but it doesn't have any Light Components. \nPlease remove the Actor or add a Light to it." (`KismetSystemLibrary.GetDisplayName` (`self.GetOwner`)) (`KismetSystemLibrary.GetDisplayName` _array_element)) true true (struct :`R` 1.0 :`A` 1.0) 500.0)))))

(fn `StopLightIgnition`
  (`self.SetComponentTickEnabled` false)
  ;[1 1 1] Make sure the final intensity is still set up properly
  (for (_array_element _array_index) (`self.LightsToChange`)
    (`LightComponent.SetIntensity` _array_element (`|GetArrayItem` (`self.LightsTargetIntensity`) _array_index))))

(fn `UpdateAllLights`
  (locals (NormalizedIntensity :type "Float (single-precision)" :default 0.0))
  (set `local.NormalizedIntensity` (`CurveFloat.GetFloatValue` (`self.CurveToFollow`) (/ (`self.CurrentChangeTime`) (`self.TransitionTime`))))
  (for (_array_element _array_index) (`self.LightsToChange`)
    (`LightComponent.SetIntensity` _array_element (* (`|GetArrayItem` (`self.LightsTargetIntensity`) _array_index) (`local.NormalizedIntensity`)))))