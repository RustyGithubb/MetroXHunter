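; BP_Metro is a test of a modular metro assembled from back cabin, shuttle and transition pieces.
; On BeginPlay, the BackCabin flag switches BackCabinChildren collision between QueryAndPhysics and none.
; The construction script is disconnected: its logic to fill the three piece arrays and toggle back cabin visibility never runs.
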(event `self.ReceiveBeginPlay`
  (bind _backcabin_children (`self.BackCabin_Children`))
  (if (`self.Back Cabin`)
    (`PrimitiveComponent.SetCollisionEnabled` _backcabin_children "QueryAndPhysics")
    (else
      (`PrimitiveComponent.SetCollisionEnabled` _backcabin_children "NoCollision"))))

(fn `UserConstructionScript`
  ;[1 1 1 0.33] Some test about a modular metro
)