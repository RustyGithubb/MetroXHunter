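; An interactable camera actor that switches the player's view to itself for close inspection, with an optional translate overlay.
; On interact, it hides the character, freezes interaction, blends the view, pushes an interact widget on the HUD viewport, swaps input mapping and notifies its trigger receiver components.
; Translate input pushes the translate widget.
; Return either backs out to the interact widget or restores the character, camera, input and UI.
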(event `self.ReceiveBeginPlay`
  ;[1 0 0 0.33 30] BEGIN PLAY
  (`KismetSystemLibrary.DelayUntilNextTick`)
  (set `self.Viewport` (`/Game/Design/_GameManagement/Core/BP_MetroHUD.Viewport` (cast `/Game/Design/_GameManagement/Core/BP_MetroHUD` (`PlayerController.GetHUD` (`GameplayStatics.GetPlayerController` 0)) :!pure true)))
  (set `self.MyTriggerComponents` (`self.K2_GetComponentsByClass` "/Game/Design/EnvironmentEvents/Components/BP_TriggerEventReceiver_Component.BP_TriggerEventReceiver_Component_C")))

(event `self.InteractableComponent.OnInteract`
  (bind _returnvalue (`GameplayStatics.GetPlayerController` 0))
  (`self.SetActorHiddenInGame` (`GameplayStatics.GetPlayerCharacter` 0) true)
  ;[0 0 0] CAMERA / PLAYER BEHAVIOR
  (`PlayerController.SetViewTargetWithBlend` (`GameplayStatics.GetPlayerController` 0) self 0.0 "VTBlend_Linear" 0.0 false)
  (`self.SetInteractionFreezed` true)
  ;[1 1 1] WIDGET
  (`/Game/Design/Widgets/WBP_Viewport.Push Widget Simple` (`self.Viewport`) "/Game/Design/Widgets/MainMenu/Interaction/WBPC_Interact.WBPC_Interact_C")
  ;[0 0 0] Input mapping Context
  (`KismetSystemLibrary.Delay` 0.2)
  (message `PlayerInputHandler.SetInputMappingContext` _returnvalue "/Game/Design/_GameManagement/Input/Player/IMC_CameraInteraction.IMC_CameraInteraction")
  (`self.EnableInput` _returnvalue) ; NOTE: This is required to give input\nevents to this actor
  ;[1 1 1 0.33] Comment
  (for _array_element (`self.MyTriggerComponents`)
    (`/Game/Design/EnvironmentEvents/Components/BP_TriggerEventReceiver_Component.OnTriggerBoxEnter` _array_element self)))

(event `EnhancedInput|/Game/Design/_GameManagement/Input/Player/IA_Return`
  (params (ActionValue :type "Float (double-precision)") (ElapsedSeconds :type "Float (double-precision)") (TriggeredSeconds :type "Float (double-precision)") (InputAction :type "InputAction Object Reference" :default "/Game/Design/_GameManagement/Input/Player/IA_Return.IA_Return"))
  (bind _returnvalue (`GameplayStatics.GetPlayerController` 0))
  (:`Started`
    (if (`self.IsTranlate`)
      (set `self.IsTranlate` false)
      ;[1 1 1] WIDGET
      (`/Game/Design/Widgets/WBP_Viewport.Push Widget Simple` (`self.Viewport`) "/Game/Design/Widgets/MainMenu/Interaction/WBPC_Interact.WBPC_Interact_C")
      (else
        (`self.SetActorHiddenInGame` (`GameplayStatics.GetPlayerCharacter` 0) false)
        ;[0 0 0 0.33 20] CAMERA PLAYER BEHAVIOR
        (`self.SetInteractionFreezed` false)
        (`PlayerController.SetViewTargetWithBlend` (`GameplayStatics.GetPlayerController` 0) (`GameplayStatics.GetPlayerCharacter` 0) 0.0 "VTBlend_Linear" 0.0 false)
        ;[0 0 0] INPUT
        (message `PlayerInputHandler.ResetInputMappingContext` _returnvalue)
        (`self.DisableInput` _returnvalue)
        ;[1 1 1] WIDGET
        (`/Game/Design/Widgets/WBP_Viewport.Clear Simple Stack` (`self.Viewport`))))))

(event `EnhancedInput|/Game/Design/_GameManagement/Input/Player/IA_Translate`
  (params (ActionValue :type "Float (double-precision)") (ElapsedSeconds :type "Float (double-precision)") (TriggeredSeconds :type "Float (double-precision)") (InputAction :type "InputAction Object Reference" :default "/Game/Design/_GameManagement/Input/Player/IA_Translate.IA_Translate"))
  (:`Started`
    (if (not (`self.IsTranlate`))
      ;[1 1 1] Push Translate
      (set `self.IsTranlate` true)
      (`/Game/Design/Widgets/WBP_Viewport.Push Widget Simple` (`self.Viewport`) (`self.Translate widget`)))))

(fn `UserConstructionScript`)