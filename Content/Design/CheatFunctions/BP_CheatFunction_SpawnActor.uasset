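; Cheat function that spawns an actor from a list of soft classes where the player camera's visibility trace hits.
; OnInit fills the option names from the class asset names; OnCheat only records a changed selection, spawning when it is repeated.
; Spawning async-loads the class, places the actor above the hit with yaw facing back along the trace, then sweeps it down, which needs root collision.
; On-screen text reports success or failure.
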(event `self.OnInit`
  ;[1 1 1 0.33] Auto fill value names with actor classes
  (`KismetArrayLibrary.Array_Clear` (`self.ValueNames`))
  (for _array_element (`self.ActorClasses`)
    (`KismetArrayLibrary.Array_Add` (`self.ValueNames`) (`UtilityLibrary.GetSoftObjectPathAssetName` (`KismetSystemLibrary.Conv_SoftObjRefToSoftClassPath` _array_element)))))

(event `self.OnCheat`
  ;[1 1 1 0.33] Avoid spawn when cycling through elements
  (if (== (`self.Index`) (`self.LastIndex`))
    (bind (_location _rotation) (`self.FindSpawnLocation`))
    ;[1 1 1 0.33] Load Class
    (bind _class (`|LoadAssetClass` (`|GetArrayItem` (`self.ActorClasses`) (`self.Index`)))
      (:`Completed`
        (bind _returnvalue (+ _location (0.0 0.0 100.0)))
        (bind _returnvalue_2 (`|SpawnActorFromClass` (castclass `Actor` _class :!pure true) (`KismetMathLibrary.MakeTransform` _returnvalue _rotation) "AdjustIfPossibleButAlwaysSpawn" "MultiplyWithRoot" null null))
        (`/Engine/EditorBlueprintResources/StandardMacros.IsValid` _returnvalue_2
          (:`Is Valid`
            (`Actor.K2_SetActorLocation` _returnvalue_2 _location true false) ; Drop to floor with Sweep enabled\nNOTE: Doesn't work if the root component doesn't have collisions
            (bind _returnvalue_3 (`KismetStringLibrary.Conv_VectorToString` _returnvalue))
            (`KismetSystemLibrary.PrintText` (`|FormatText` "CheatFunction_SpawnActor: Spawned '{Actor}' at {Location}" _returnvalue_2 _returnvalue_3) true true (struct :`G` 0.66 :`B` 1.0 :`A` 1.0) 3.0))
          (:`Is Not Valid`
            (`KismetSystemLibrary.PrintText` (`|FormatText` "CheatFunction_SpawnActor: Failed to spawn '{ActorClass}' at {Location}, try another location" (`KismetSystemLibrary.GetClassDisplayName` _class) _returnvalue_3) true true (struct :`R` 1.0 :`A` 1.0) 3.0)))))
    (else
      (set `self.LastIndex` (`self.Index`)))))

(fn `FindSpawnLocation`
  (returns (Location :type "Vector Structure") (Rotation :type "Rotator Structure"))
  (bind _playercameramanager (`PlayerController.PlayerCameraManager` (`CheatManager.GetPlayerController` (`self.CheatManager`))))
  (bind _returnvalue (`Actor.GetActorForwardVector` _playercameramanager))
  (bind _outhit (`KismetSystemLibrary.LineTraceSingle` (+ (`PlayerCameraManager.GetCameraLocation` _playercameramanager) (* _returnvalue 50.0)) (* _returnvalue 500000.0) "TraceTypeQuery1"))
  (bind (_bblockinghit _binitialoverlap _time _distance _location _impactpoint _normal _impactnormal _physmat _hitactor _hitcomponent _hitbonename _bonename _hititem _elementindex _faceindex _tracestart _traceend) (`GameplayStatics.BreakHitResult` _outhit))
  (bind (_returnvalue_roll _returnvalue_pitch _returnvalue_yaw) (`KismetMathLibrary.BreakRotator` (`KismetMathLibrary.FindLookAtRotation` _traceend _tracestart)))
  (return _location (`KismetMathLibrary.MakeRotator` 0.0 0.0 _returnvalue_yaw)))