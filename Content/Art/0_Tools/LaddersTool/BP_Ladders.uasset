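; BP_Ladders is an art tool actor that builds ladders or stair-like runs by repeating a static mesh along a spline.
; The construction script adds one mesh component per LenghtBetweenSteps interval of spline length, placed and rotated to the spline in local space.
; Where the spline's world-space tangent does not point upward, it adds a 180-degree yaw so steps on flat or descending sections are flipped.
; It has no runtime logic.
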(fn `UserConstructionScript`
  (bind _spline (`self.Spline`))
  (for _index (range (`.ReturnValue` (`KismetMathLibrary.FMod` (`SplineComponent.GetSplineLength` (`self.Spline`)) (`self.LenghtBetweenSteps`))))
    (bind _returnvalue (`AddComponent|NODE_AddStaticMeshComponent-0`))
    (bind _returnvalue_2 (* _index (`self.LenghtBetweenSteps`)))
    (if (> (.z (`SplineComponent.GetTangentAtDistanceAlongSpline` (`self.Spline`) _returnvalue_2 "World")) 0.0)
      (bind _returnvalue_3 (`SplineComponent.GetLocationAtDistanceAlongSpline` _spline _returnvalue_2 "Local"))
      (bind _returnvalue_4 (`SplineComponent.GetRotationAtDistanceAlongSpline` _spline _returnvalue_2 "Local"))
      (`SceneComponent.K2_SetRelativeLocationAndRotation` _returnvalue _returnvalue_3 _returnvalue_4 false false)
      (else
        (`SceneComponent.K2_SetRelativeLocationAndRotation` _returnvalue _returnvalue_3 (`KismetMathLibrary.ComposeRotators` _returnvalue_4 (struct :`Pitch` 180.0)) false false)))))