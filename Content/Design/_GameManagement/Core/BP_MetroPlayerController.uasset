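; Metro player controller that handles pausing, input freezing and debug tools.
; On BeginPlay it caches the custom cheat manager and HUD, enabling cheat input for the HUD-driven cheat menu and Spacebar noclip cancel.
; The pause action opens a widget that unpauses on deactivation, and freezing swaps mapping contexts.
; Gamepad buttons feed the input visualizer by event, while sticks and triggers are polled on Tick so zero values still register.
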(event Custom|SendControllerVisualizerData
  (bind _returnvalue (PlayerController|LocalPlayerSubsystems|GetEnhancedInputLocalPlayerSubsystem))
  ;[0 0 0 0.33 50] ControllerVisualizer Debug
  ;;[0.08067 0.6955 1 0.33] Stick Movement & Trigger Axes
  (Utilities|IsValid _returnvalue
    (:Is%20Valid
      (if (.ReturnValue (Class|EnhancedInputSubsystemInterface|HasMappingContext _returnvalue "/Game/Design/_GameManagement/Input/Visualizer/IMC_ControllerVisualizer.IMC_ControllerVisualizer"))
        (bind _controllerinputvisualizer (Variables|Default|GetControllerInputVisualizer)
          (:then
            (Default|ReceiveInputVisualizationDataStick _controllerinputvisualizer (Input|EnhancedActionValues|GetIA_Visu_StickLeft_Movement) true)
            (Default|ReceiveInputVisualizationDataStick (Variables|Default|GetControllerInputVisualizer) (Input|EnhancedActionValues|GetIA_Visu_StickRight_Movement) false)
            (Default|ReceiveInputVisualizationDataAxis (Variables|Default|GetControllerInputVisualizer) (Input|EnhancedActionValues|GetIA_Visu_Trigger_Left) true)
            (Default|ReceiveInputVisualizationDataAxis (Variables|Default|GetControllerInputVisualizer) (Input|EnhancedActionValues|GetIA_Visu_Trigger_Right) false))
          (:else))))))

(event Custom|OnPauseMenuWidgetDeactivated
  (Game|SetGamePaused false))

(event Input|EnhancedActionEvents|EnhancedInputActionIA_CheatMenu
  (params (ActionValue :type Boolean) (ElapsedSeconds :type Float%20%28double-precision%29) (TriggeredSeconds :type Float%20%28double-precision%29) (InputAction :type Input%20Action%20Object%20Reference :default "/Game/Design/_GameManagement/Input/IA_CheatMenu.IA_CheatMenu"))
  (:Completed
    (CallFunction|ShowCheatMenu false true)))

(event Input|EnhancedActionEvents|EnhancedInputActionIA_Visu_FaceButton_Top
  (params (ActionValue :type Boolean) (ElapsedSeconds :type Float%20%28double-precision%29) (TriggeredSeconds :type Float%20%28double-precision%29) (InputAction :type Input%20Action%20Object%20Reference :default "/Game/Design/_GameManagement/Input/Visualizer/IA_Visu_FaceButton_Top.IA_Visu_FaceButton_Top"))
  ;[0 0 0 0.33 50] ControllerVisualizer Debug
  ;;[1 0.5477 0.8376 0.33] Face Button
  (:Started
    (Default|ReceiveInputVisualizationDataButton (Variables|Default|GetControllerInputVisualizer) true "NewEnumerator7"))
  (:Completed
    (Default|ReceiveInputVisualizationDataButton (Variables|Default|GetControllerInputVisualizer) false "NewEnumerator7")))

(event Input|EnhancedActionEvents|EnhancedInputActionIA_Visu_FaceButton_Left
  (params (ActionValue :type Boolean) (ElapsedSeconds :type Float%20%28double-precision%29) (TriggeredSeconds :type Float%20%28double-precision%29) (InputAction :type Input%20Action%20Object%20Reference :default "/Game/Design/_GameManagement/Input/Visualizer/IA_Visu_FaceButton_Left.IA_Visu_FaceButton_Left"))
  ;[0 0 0 0.33 50] ControllerVisualizer Debug
  ;;[1 0.5477 0.8376 0.33] Face Button
  (:Started
    (Default|ReceiveInputVisualizationDataButton (Variables|Default|GetControllerInputVisualizer) true "NewEnumerator5"))
  (:Completed
    (Default|ReceiveInputVisualizationDataButton (Variables|Default|GetControllerInputVisualizer) false "NewEnumerator5")))

(event Input|EnhancedActionEvents|EnhancedInputActionIA_Visu_FaceButton_Right
  (params (ActionValue :type Boolean) (ElapsedSeconds :type Float%20%28double-precision%29) (TriggeredSeconds :type Float%20%28double-precision%29) (InputAction :type Input%20Action%20Object%20Reference :default "/Game/Design/_GameManagement/Input/Visualizer/IA_Visu_FaceButton_Right.IA_Visu_FaceButton_Right"))
  ;[0 0 0 0.33 50] ControllerVisualizer Debug
  ;;[1 0.5477 0.8376 0.33] Face Button
  (:Started
    (Default|ReceiveInputVisualizationDataButton (Variables|Default|GetControllerInputVisualizer) true "NewEnumerator6"))
  (:Completed
    (Default|ReceiveInputVisualizationDataButton (Variables|Default|GetControllerInputVisualizer) false "NewEnumerator6")))

(event Input|EnhancedActionEvents|EnhancedInputActionIA_Visu_DPad_Bottom
  (params (ActionValue :type Boolean) (ElapsedSeconds :type Float%20%28double-precision%29) (TriggeredSeconds :type Float%20%28double-precision%29) (InputAction :type Input%20Action%20Object%20Reference :default "/Game/Design/_GameManagement/Input/Visualizer/IA_Visu_DPad_Bottom.IA_Visu_DPad_Bottom"))
  ;[0 0 0 0.33 50] ControllerVisualizer Debug
  ;;[0.3557 1 0.4036 0.33] DPad
  (:Started
    (Default|ReceiveInputVisualizationDataButton (Variables|Default|GetControllerInputVisualizer) true "NewEnumerator0"))
  (:Completed
    (Default|ReceiveInputVisualizationDataButton (Variables|Default|GetControllerInputVisualizer) false "NewEnumerator0")))

(event Input|EnhancedActionEvents|EnhancedInputActionIA_Visu_DPad_Left
  (params (ActionValue :type Boolean) (ElapsedSeconds :type Float%20%28double-precision%29) (TriggeredSeconds :type Float%20%28double-precision%29) (InputAction :type Input%20Action%20Object%20Reference :default "/Game/Design/_GameManagement/Input/Visualizer/IA_Visu_DPad_Left.IA_Visu_DPad_Left"))
  ;[0 0 0 0.33 50] ControllerVisualizer Debug
  ;;[0.3557 1 0.4036 0.33] DPad
  (:Started
    (Default|ReceiveInputVisualizationDataButton (Variables|Default|GetControllerInputVisualizer) true "NewEnumerator1"))
  (:Completed
    (Default|ReceiveInputVisualizationDataButton (Variables|Default|GetControllerInputVisualizer) false "NewEnumerator1")))

(event Input|EnhancedActionEvents|EnhancedInputActionIA_Visu_Special_Left
  (params (ActionValue :type Boolean) (ElapsedSeconds :type Float%20%28double-precision%29) (TriggeredSeconds :type Float%20%28double-precision%29) (InputAction :type Input%20Action%20Object%20Reference :default "/Game/Design/_GameManagement/Input/Visualizer/IA_Visu_Special_Left.IA_Visu_Special_Left"))
  ;[0 0 0 0.33 50] ControllerVisualizer Debug
  ;;[0.6146 0.6146 0.6146 0.33] Special Buttons
  (:Started
    (Default|ReceiveInputVisualizationDataButton (Variables|Default|GetControllerInputVisualizer) true "NewEnumerator10"))
  (:Completed
    (Default|ReceiveInputVisualizationDataButton (Variables|Default|GetControllerInputVisualizer) false "NewEnumerator10")))

(event Input|EnhancedActionEvents|EnhancedInputActionIA_TPS_Pause
  (params (ActionValue :type Boolean) (ElapsedSeconds :type Float%20%28double-precision%29) (TriggeredSeconds :type Float%20%28double-precision%29) (InputAction :type Input%20Action%20Object%20Reference :default "/TPS_FeedlingAddon/TPS/_Input/IA_TPS_Pause.IA_TPS_Pause"))
  (:Started
    (bind _returnvalue (UserInterface|CreateWidget "/Game/Design/Widgets/Menu_Pause/WBPC_GeneralPause.WBPC_GeneralPause_C"))
    (UserInterface|Viewport|AddtoViewport _returnvalue 0)
    (Game|SetGamePaused true)
    (EventDispatchers|BindEventtoBPonWidgetDeactivated _returnvalue (delegate Custom|OnPauseMenuWidgetDeactivated))))

(event Input|EnhancedActionEvents|EnhancedInputActionIA_Visu_Special_Right
  (params (ActionValue :type Boolean) (ElapsedSeconds :type Float%20%28double-precision%29) (TriggeredSeconds :type Float%20%28double-precision%29) (InputAction :type Input%20Action%20Object%20Reference :default "/Game/Design/_GameManagement/Input/Visualizer/IA_Visu_Special_Right.IA_Visu_Special_Right"))
  ;[0 0 0 0.33 50] ControllerVisualizer Debug
  ;;[0.6146 0.6146 0.6146 0.33] Special Buttons
  (:Started
    (Default|ReceiveInputVisualizationDataButton (Variables|Default|GetControllerInputVisualizer) true "NewEnumerator11"))
  (:Completed
    (Default|ReceiveInputVisualizationDataButton (Variables|Default|GetControllerInputVisualizer) false "NewEnumerator11")))

(event Input|EnhancedActionEvents|EnhancedInputActionIA_Visu_Shoulder_Left
  (params (ActionValue :type Boolean) (ElapsedSeconds :type Float%20%28double-precision%29) (TriggeredSeconds :type Float%20%28double-precision%29) (InputAction :type Input%20Action%20Object%20Reference :default "/Game/Design/_GameManagement/Input/Visualizer/IA_Visu_Shoulder_Left.IA_Visu_Shoulder_Left"))
  ;[0 0 0 0.33 50] ControllerVisualizer Debug
  ;;[0.9995 1 0.2907 0.33] Shoulder Buttons
  (:Started
    (Default|ReceiveInputVisualizationDataButton (Variables|Default|GetControllerInputVisualizer) true "NewEnumerator8"))
  (:Completed
    (Default|ReceiveInputVisualizationDataButton (Variables|Default|GetControllerInputVisualizer) false "NewEnumerator8")))

(event Input|EnhancedActionEvents|EnhancedInputActionIA_Visu_Shoulder_Right
  (params (ActionValue :type Boolean) (ElapsedSeconds :type Float%20%28double-precision%29) (TriggeredSeconds :type Float%20%28double-precision%29) (InputAction :type Input%20Action%20Object%20Reference :default "/Game/Design/_GameManagement/Input/Visualizer/IA_Visu_Shoulder_Right.IA_Visu_Shoulder_Right"))
  ;[0 0 0 0.33 50] ControllerVisualizer Debug
  ;;[0.9995 1 0.2907 0.33] Shoulder Buttons
  (:Started
    (Default|ReceiveInputVisualizationDataButton (Variables|Default|GetControllerInputVisualizer) true "NewEnumerator9"))
  (:Completed
    (Default|ReceiveInputVisualizationDataButton (Variables|Default|GetControllerInputVisualizer) false "NewEnumerator9")))

(event Input|EnhancedActionEvents|EnhancedInputActionIA_Visu_StickLeft_Press
  (params (ActionValue :type Boolean) (ElapsedSeconds :type Float%20%28double-precision%29) (TriggeredSeconds :type Float%20%28double-precision%29) (InputAction :type Input%20Action%20Object%20Reference :default "/Game/Design/_GameManagement/Input/Visualizer/IA_Visu_StickLeft_Press.IA_Visu_StickLeft_Press"))
  ;[0 0 0 0.33 50] ControllerVisualizer Debug
  ;;[0.1729 0.2596 1 0.33] Stick Presses
  (:Started
    (Default|ReceiveInputVisualizationDataButton (Variables|Default|GetControllerInputVisualizer) true "NewEnumerator12"))
  (:Completed
    (Default|ReceiveInputVisualizationDataButton (Variables|Default|GetControllerInputVisualizer) false "NewEnumerator12")))

(event Input|EnhancedActionEvents|EnhancedInputActionIA_Visu_StickRight_Press
  (params (ActionValue :type Boolean) (ElapsedSeconds :type Float%20%28double-precision%29) (TriggeredSeconds :type Float%20%28double-precision%29) (InputAction :type Input%20Action%20Object%20Reference :default "/Game/Design/_GameManagement/Input/Visualizer/IA_Visu_StickRight_Press.IA_Visu_StickRight_Press"))
  ;[0 0 0 0.33 50] ControllerVisualizer Debug
  ;;[0.1729 0.2596 1 0.33] Stick Presses
  (:Started
    (Default|ReceiveInputVisualizationDataButton (Variables|Default|GetControllerInputVisualizer) true "NewEnumerator13"))
  (:Completed
    (Default|ReceiveInputVisualizationDataButton (Variables|Default|GetControllerInputVisualizer) false "NewEnumerator13")))

(event Input|EnhancedActionEvents|EnhancedInputActionIA_Visu_DPad_Right
  (params (ActionValue :type Boolean) (ElapsedSeconds :type Float%20%28double-precision%29) (TriggeredSeconds :type Float%20%28double-precision%29) (InputAction :type Input%20Action%20Object%20Reference :default "/Game/Design/_GameManagement/Input/Visualizer/IA_Visu_DPad_Right.IA_Visu_DPad_Right"))
  ;[0 0 0 0.33 50] ControllerVisualizer Debug
  ;;[0.3557 1 0.4036 0.33] DPad
  (:Started
    (Default|ReceiveInputVisualizationDataButton (Variables|Default|GetControllerInputVisualizer) true "NewEnumerator2"))
  (:Completed
    (Default|ReceiveInputVisualizationDataButton (Variables|Default|GetControllerInputVisualizer) false "NewEnumerator2")))

(event Input|EnhancedActionEvents|EnhancedInputActionIA_Visu_DPad_Top
  (params (ActionValue :type Boolean) (ElapsedSeconds :type Float%20%28double-precision%29) (TriggeredSeconds :type Float%20%28double-precision%29) (InputAction :type Input%20Action%20Object%20Reference :default "/Game/Design/_GameManagement/Input/Visualizer/IA_Visu_DPad_Top.IA_Visu_DPad_Top"))
  ;[0 0 0 0.33 50] ControllerVisualizer Debug
  ;;[0.3557 1 0.4036 0.33] DPad
  (:Started
    (Default|ReceiveInputVisualizationDataButton (Variables|Default|GetControllerInputVisualizer) true "NewEnumerator3"))
  (:Completed
    (Default|ReceiveInputVisualizationDataButton (Variables|Default|GetControllerInputVisualizer) false "NewEnumerator3")))

(event Input|EnhancedActionEvents|EnhancedInputActionIA_Visu_FaceButton_Bottom
  (params (ActionValue :type Boolean) (ElapsedSeconds :type Float%20%28double-precision%29) (TriggeredSeconds :type Float%20%28double-precision%29) (InputAction :type Input%20Action%20Object%20Reference :default "/Game/Design/_GameManagement/Input/Visualizer/IA_Visu_FaceButton_Bottom.IA_Visu_FaceButton_Bottom"))
  ;[0 0 0 0.33 50] ControllerVisualizer Debug
  ;;[1 0.5477 0.8376 0.33] Face Button
  (:Started
    (Default|ReceiveInputVisualizationDataButton (Variables|Default|GetControllerInputVisualizer) true "NewEnumerator4"))
  (:Completed
    (Default|ReceiveInputVisualizationDataButton (Variables|Default|GetControllerInputVisualizer) false "NewEnumerator4")))

(event EventToggleFreezePlayer
  (params (bShouldFreeze :type Boolean))
  (if bShouldFreeze
    (Class|PlayerInputHandler|SetInputMappingContext "/Game/Design/_GameManagement/Input/Player/IMC_None.IMC_None")
    (else
      (Class|PlayerInputHandler|ResetInputMappingContext))))

(event EventTick
  (params (DeltaSeconds :type Float%20%28single-precision%29))
  (CallFunction|SendControllerVisualizerData) ; Send stick & axes values on an Event Tick,\nbecause otherwise it won't send anything\non the frames where the values are 0,\nand the visualizer will be wrong
)

(event EventBeginPlay
  (Init|GetReferences)
  (Variables|Default|GetCustomCheatManager
    (:then
      (Input|AddMappingContext (PlayerController|LocalPlayerSubsystems|GetEnhancedInputLocalPlayerSubsystem) "/Game/Design/_GameManagement/Input/IMC_Cheat.IMC_Cheat" 0 "(bIgnoreAllPressedKeysUntilRelease=True,bForceImmediately=False,bNotifyUserSettings=False)"))
    (:else)))

(event Input|KeyboardEvents|DebugKeySpaceBar
  (params (Key :type Key%20Structure :default "None") (ActionValue :type Input%20Action%20Value%20Structure))
  ;[1 1 1 0.33] Cancel Noclip with Spacebar
  (:Pressed
    (bind _customcheatmanager (Variables|Default|GetCustomCheatManager)
      (:then
        (if (Utilities|Enum|NotEqual(Enum) (Variables|/Script/Engine.CharacterMovementComponent|GetMovementMode (Variables|/Script/Engine.Character|GetCharacterMovement (Game|GetPlayerCharacter 0))) "MOVE_Walking")
          (Class|CheatManager|Walk _customcheatmanager)))
      (:else))))

(fn ConstructionScript)

(fn CreateViewport
  ;[1 1 1 0.33] DOP - This is now managed by the HUD
)

(fn GetReferences
  (bind _asbp_metro_cheat_manager (Utilities|Casting|CastToBP_MetroCheatManager (Variables|Default|GetCheatManager)))
  (Variables|Default|SetCustomCheatManager _asbp_metro_cheat_manager) ; This is a Free Reference since this\nis set in the Class Defaults
  (Variables|Default|SetGeneralHUD (HUD|GetHUD)))

(fn ShowCheatMenu
  (params (NewVisibility :type Boolean) (ShouldToggle :type Boolean))
  (Class|MainHUD|ShowHideCheatMenuVisibility(Message) (Variables|Default|GetGeneralHUD) (Variables|Default|GetCustomCheatManager) self NewVisibility ShouldToggle))