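; Test actor that repeatedly applies fluid force impulses at its own location to a fluid simulation.
; On BeginPlay it caches the first BP_FluidSim_01 in the level.
; Tick runs a fixed time step that sends the configured impulse settings, stamped with the actor's world position, at a set interval.
; A Trigger event re-finds the simulation and fires a single impulse on demand.
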(event `self.ReceiveBeginPlay`
  (bind _outactors (`GameplayStatics.GetAllActorsOfClass` "/Water/FluidSimulation/Blueprints/BP_FluidSim_01.BP_FluidSim_01_C"))
  (set `self.Sim` (`|GetArrayItem` _outactors)))

(event `self.ReceiveTick`
  (params (DeltaSeconds :type "Float (single-precision)"))
  (bind _sim (`self.Sim`))
  (`/Water/FluidSimulation/Blueprints/Libraries/PhysicsMacros.Fixed Time Step` (`self.Impulse Every N Seconds`)
    (:`Fixed Step Execution`
      (bind _structout (setmembers `/Water/FluidSimulation/Blueprints/Structs/FluidForceImpulse` :`StructRef` (`self.Imulse Settings`) :`World Position` (`self.K2_GetActorLocation`) :!label _label))
      (`/Engine/EditorBlueprintResources/StandardMacros.IsValid` _sim
        (:`Is Valid`
          (`/Water/FluidSimulation/Blueprints/BP_FluidSim_01.Apply Fluid Force Impulse` _sim _structout))))))

(event `Trigger`
  (bind _outactors (`GameplayStatics.GetAllActorsOfClass` "/Water/FluidSimulation/Blueprints/BP_FluidSim_01.BP_FluidSim_01_C"))
  (set `self.Sim` (`|GetArrayItem` _outactors))
  (goto _label))

(fn `UserConstructionScript`)