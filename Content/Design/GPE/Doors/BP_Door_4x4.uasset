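; Double swing door Blueprint that opens with metal door sounds and, once open, removes its interaction component.
; Box overlaps call OnDoorHit, while SetDoorOpened plays a timeline rotating both leaves in opposite yaw from their starting angles; it has no closing branch.
; The construction script uses FlipRotation to choose swing direction, mesh offset and arrow facing.
; CloseDoorEditor snaps both leaves back to zero rotation.
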(event `self.ReceiveBeginPlay`
  (bind (_relativerotation_roll _relativerotation_pitch _relativerotation_yaw) (`KismetMathLibrary.BreakRotator` (`SceneComponent.RelativeRotation` (`self.R_Door`))))
  (bind (_relativerotation_roll_2 _relativerotation_pitch_2 _relativerotation_yaw_2) (`KismetMathLibrary.BreakRotator` (`SceneComponent.RelativeRotation` (`self.L_Door`))))
  (set `self.LStartYawRotation` _relativerotation_yaw_2)
  (set `self.RStartYawRotation` _relativerotation_yaw))

(event `self.Box.OnComponentBeginOverlap`
  (params (OverlappedComponent :type "PrimitiveComponent Object Reference") (OtherActor :type "Actor Object Reference") (OtherComp :type "PrimitiveComponent Object Reference") (OtherBodyIndex :type Integer) (bFromSweep :type Boolean) (SweepResult :type "HitResult Structure (by ref)"))
  (`self.OnDoorHit` OtherActor))

(event `self.SetDoorOpened`
  (params (bShouldOpen :type Boolean))
  (if bShouldOpen
    (`GameplayStatics.PlaySoundAtLocation` "/Game/Sounds/Audio/SFX/SFX_GPE/SFX_Door/SC_MetalDoor_Opening.SC_MetalDoor_Opening" (`SceneComponent.K2_GetComponentLocation` (`self.R_Door`)) (struct) 1.0 1.0 0.0 null null null null)
    (`GameplayStatics.PlaySoundAtLocation` "/Game/Sounds/Audio/SFX/SFX_GPE/SFX_Door/SC_MetalDoor_Opening.SC_MetalDoor_Opening" (`SceneComponent.K2_GetComponentLocation` (`self.L_AudioPos`)) (struct) 1.0 1.0 0.0 null null null null)
    (bind (_direction _rotation) (`Timeline|OpenDoor` :!via `PlayFromStart`)
      (:`Update`
        (`SceneComponent.K2_SetRelativeRotation` (`self.L_Door`) (`KismetMathLibrary.MakeRotator` 0.0 0.0 (+ (* _rotation (`self.FinalRotation`)) (`self.LStartYawRotation`))) false false)
        (`SceneComponent.K2_SetRelativeRotation` (`self.R_Door`) (`KismetMathLibrary.MakeRotator` 0.0 0.0 (+ (* _rotation (* (`self.FinalRotation`) -1.0)) (`self.RStartYawRotation`))) false false))
      (:`Finished`
        (set `self.bIsOpened` true)
        (`self.InteractableComponent`
          (:`then`
            (`self.SetInteractionFreezed` true)
            (`self.RemoveInteractionComponent`))
          (:`else`))))))

(event `self.CloseDoorEditor`
  (`SceneComponent.K2_SetRelativeRotation` (`self.L_Door`) (`KismetMathLibrary.MakeRotator` 0.0) false false)
  (`SceneComponent.K2_SetRelativeRotation` (`self.R_Door`) (`KismetMathLibrary.MakeRotator` 0.0) false false))

(fn `UserConstructionScript`
  (if (`self.bFlipRotation`)
    (set `self.FinalRotation` (`self.TargetRotation`))
    (`SceneComponent.K2_SetRelativeLocation` (`self.StaticMesh`) (0.0 -150.0 0.0) false false)
    (`SceneComponent.K2_SetRelativeRotation` :`self` (`self.Arrow`))
    (else
      (set `self.FinalRotation` (* (`self.TargetRotation`) -1.0))
      (`SceneComponent.K2_SetRelativeLocation` (`self.StaticMesh`) (-40.0 -150.0 0.0) false false)
      (`SceneComponent.K2_SetRelativeRotation` (`self.Arrow`) (struct :`Yaw` -180.0) false false))))