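; BP_Destructible_LightBulbe is a destructible light bulb with a spotlight that supports flickering.
; On damage, it swaps the sphere mesh for the hidden GCTEST geometry collection, destroys the spotlight and calls its destroy logic.
; Construction registers a child-actor anchor field with that collection.
; Flicker callbacks expose the spotlight, swap bulb materials and zero intensity on stop, while the per-update emissive scaling is left unwired.
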(event `self.Health.OnDamage`
  (params (DamageContext :type "DamageContext Structure (by ref)"))
  (`SceneComponent.SetHiddenInGame` (`self.GC_TEST`) false false)
  (`SceneComponent.SetHiddenInGame` (`self.Sphere`) true false)
  (`ActorComponent.K2_DestroyComponent` (`self.SpotLight`))
  (`self.OnDestroy`))

(fn `OnFlickLightStart`
  (params (LightData :type "LightData Structure (by ref)"))
  (`PrimitiveComponent.SetMaterial` (`self.Sphere`) 0 "/Game/Design/GPE/Destructible/MI_BulbeTEST.MI_BulbeTEST")
  (setmembers `LightData` :`StructRef` LightData :`OriginalLightIntensity` 5000.0)
  (return))

(fn `OnFlickLightStop`
  (params (LightData :type "LightData Structure (by ref)"))
  (`PrimitiveComponent.SetMaterial` (`self.Sphere`) 0 "/Game/Art/Materials/Material_Instance/MI_Neon_White.MI_Neon_White")
  (`LightComponent.SetIntensity` (`self.SpotLight`) 0.0)
  (return))

(fn `OnFlickLightTick`
  (params (DeltaTime :type "Float (single-precision)") (LightData :type "LightData Structure (by ref)"))
  (return))

(fn `OnFlickLightUpdate`
  (params (LightData :type "LightData Structure (by ref)") (IntensityScale :type "Float (single-precision)"))
  (if (== null (`.LightComponent` (break `LightData` LightData)))
    _))

(fn `RetrieveFlickableLights`
  (returns (ReturnValue :type "Array of LightComponent Object Reference"))
  (return (`|MakeArray` (`self.SpotLight`) :!type "LightComponent Object Reference")))

(fn `UserConstructionScript`
  (`PrimitiveComponent.SetMaterial` (`self.Sphere`) 0 (`self.LightMaterial`))
  (`SceneComponent.SetHiddenInGame` (`self.GC_TEST`) true false)
  (bind _asfs_anchor_field_generic (cast `/Engine/EditorResources/FieldNodes/FS_AnchorField_Generic` (`ChildActorComponent.ChildActor` (`self.ChildActor`))))
  (`KismetArrayLibrary.Array_Add` (`GeometryCollectionComponent.InitializationFields` (`self.GC_TEST`)) _asfs_anchor_field_generic))