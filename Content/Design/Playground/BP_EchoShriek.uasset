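; BP_EchoShriek is an actor that answers shrieks it receives with a faint echoing creature shriek.
; Its shriek receiver component supplies the emission origin and radius, and the actor responds only when it is roughly in the outer quarter of that radius or beyond.
; The reply plays at the actor's location with randomized low volume and varied pitch, using tunnel echo attenuation.
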(event `self.BP_ShriekReceiverComponent.OnShriekReceived`
  (params (EmissionContext :type "/Game/Design/Enemies/Shriek/F_ShriekEmissionContext Structure"))
  (bind (_emitter _origin _radius) (break `/Game/Design/Enemies/Shriek/F_ShriekEmissionContext` EmissionContext))
  ;[1 1 1 0.33] Only accept the request & shriek back if you're in the outer X% of the shriek radius
  (if (>= (* (`KismetMathLibrary.Vector_Distance` (`self.K2_GetActorLocation`) _origin) 1.35) _radius)
    (`GameplayStatics.PlaySoundAtLocation` "/Game/Sounds/Audio/SFX/SculkShriekers/SC_CreatureShriek.SC_CreatureShriek" (`self.K2_GetActorLocation`) (struct) (`KismetMathLibrary.RandomFloatInRange` 0.08 0.15) (`KismetMathLibrary.RandomFloatInRange` 0.75 1.35) 0.0 "/Game/Sounds/Attenuations/SA_TunnelEcho.SA_TunnelEcho" null self null)))

(fn `UserConstructionScript`)