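; Test manager for enemy AI that keeps a chosen number of BP_SmallSpider enemies alive.
; Five overlap boxes let BP_MainChara pick a target of one to five, which updates a text display and destroys all current spiders.
; A looping timer prunes dead spiders from the array and spawns one per tick, with a default controller, at the spawn location indexed by the current count until the target is met.
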(event `self.ReceiveBeginPlay`
  (`self.UpdateTargetNumberOfSpiders` 1)
  (`KismetSystemLibrary.K2_SetTimerDelegate` (delegate `VerifySpiderArrayAndSpawn`) 0.2 true))

(event `VerifySpiderArrayAndSpawn`
  (bind (_arrayindex _arrayelement) (`/Engine/EditorBlueprintResources/StandardMacros.ReverseForEachLoop` (`self.SpawnedSpiders`))
    (:`LoopBody`
      (`/Engine/EditorBlueprintResources/StandardMacros.IsValid` _arrayelement
        (:`Is Not Valid`
          (`KismetArrayLibrary.Array_Remove` (`self.SpawnedSpiders`) _arrayindex))))
    (:`Completed`
      (if (< (`KismetArrayLibrary.Array_Length` (`self.SpawnedSpiders`)) (`self.TargetNumberOfSpiders`))
        (`self.SpawnNewSpider`)))))

(event `self.1EnemyBox.OnComponentBeginOverlap`
  (params (OverlappedComponent :type "PrimitiveComponent Object Reference") (OtherActor :type "Actor Object Reference") (OtherComp :type "PrimitiveComponent Object Reference") (OtherBodyIndex :type Integer) (bFromSweep :type Boolean) (SweepResult :type "HitResult Structure (by ref)"))
  (if (`/Game/o_Libraries/BPL_GeneralUtilities.Is Actor Of Class` OtherActor "/Game/0_Design/GameManagement_/BP_MainChara.BP_MainChara_C")
    (`self.UpdateTargetNumberOfSpiders` 1)))

(event `self.2EnemyBox.OnComponentBeginOverlap`
  (params (OverlappedComponent :type "PrimitiveComponent Object Reference") (OtherActor :type "Actor Object Reference") (OtherComp :type "PrimitiveComponent Object Reference") (OtherBodyIndex :type Integer) (bFromSweep :type Boolean) (SweepResult :type "HitResult Structure (by ref)"))
  (if (`/Game/o_Libraries/BPL_GeneralUtilities.Is Actor Of Class` OtherActor "/Game/0_Design/GameManagement_/BP_MainChara.BP_MainChara_C")
    (`self.UpdateTargetNumberOfSpiders` 2)))

(event `self.3EnemyBox.OnComponentBeginOverlap`
  (params (OverlappedComponent :type "PrimitiveComponent Object Reference") (OtherActor :type "Actor Object Reference") (OtherComp :type "PrimitiveComponent Object Reference") (OtherBodyIndex :type Integer) (bFromSweep :type Boolean) (SweepResult :type "HitResult Structure (by ref)"))
  (if (`/Game/o_Libraries/BPL_GeneralUtilities.Is Actor Of Class` OtherActor "/Game/0_Design/GameManagement_/BP_MainChara.BP_MainChara_C")
    (`self.UpdateTargetNumberOfSpiders` 3)))

(event `self.4EnemyBox.OnComponentBeginOverlap`
  (params (OverlappedComponent :type "PrimitiveComponent Object Reference") (OtherActor :type "Actor Object Reference") (OtherComp :type "PrimitiveComponent Object Reference") (OtherBodyIndex :type Integer) (bFromSweep :type Boolean) (SweepResult :type "HitResult Structure (by ref)"))
  (if (`/Game/o_Libraries/BPL_GeneralUtilities.Is Actor Of Class` OtherActor "/Game/0_Design/GameManagement_/BP_MainChara.BP_MainChara_C")
    (`self.UpdateTargetNumberOfSpiders` 4)))

(event `self.5EnemyBox.OnComponentBeginOverlap`
  (params (OverlappedComponent :type "PrimitiveComponent Object Reference") (OtherActor :type "Actor Object Reference") (OtherComp :type "PrimitiveComponent Object Reference") (OtherBodyIndex :type Integer) (bFromSweep :type Boolean) (SweepResult :type "HitResult Structure (by ref)"))
  (if (`/Game/o_Libraries/BPL_GeneralUtilities.Is Actor Of Class` OtherActor "/Game/0_Design/GameManagement_/BP_MainChara.BP_MainChara_C")
    (`self.UpdateTargetNumberOfSpiders` 5)))

(fn `SpawnNewSpider`
  (bind _returnvalue (`|SpawnActorFromClass` "/Game/0_Design/EnemiesAI/SmallSpider/BP_SmallSpider.BP_SmallSpider_C" (`KismetMathLibrary.MakeTransform` (`self.K2_GetActorLocation` (`|GetArrayItem` (`self.SpawnLocations`) (`KismetArrayLibrary.Array_Length` (`self.SpawnedSpiders`))))) "Undefined" "MultiplyWithRoot" null null))
  (`KismetArrayLibrary.Array_Add` (`self.SpawnedSpiders`) _returnvalue)
  (`Pawn.SpawnDefaultController` _returnvalue))

(fn `UpdateTargetNumberOfSpiders`
  (params (NewTarget :type Integer))
  (bind _output_get (set `self.TargetNumberOfSpiders` NewTarget))
  (`TextRenderComponent.K2_SetText` (`self.TextRender`) (`|FormatText` "Target # of Spiders: {No}" _output_get))
  (for _array_element (`self.SpawnedSpiders`)
    (`self.K2_DestroyActor` _array_element)))

(fn `UserConstructionScript`)