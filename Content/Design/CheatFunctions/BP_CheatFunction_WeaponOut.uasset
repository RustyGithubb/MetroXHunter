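; Cheat function Blueprint that toggles weapon equip on the player character, BP_Charles.
; On init it waits one tick, then caches the cheat manager's controlled pawn cast to BP_Charles.
; When the cheat fires, it calls EquipWeapon on that character with the current toggle state.
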(event `self.OnInit`
  (`KismetSystemLibrary.DelayUntilNextTick`)
  (`self.GetReferences`))

(event `self.OnCheat`
  (`BaseMetroPlayerCharacter.EquipWeapon` (`self.PlayerCharacter`) (`self.bIsToggled`)))

(fn `GetReferences`
  (bind _returnvalue (`Controller.K2_GetPawn` (`CheatManager.GetPlayerController` (`self.CheatManager`))))
  (`/Engine/EditorBlueprintResources/StandardMacros.IsValid` _returnvalue
    (:`Is Valid`
      (bind _asbp_charles (cast `/Game/Developers/corentinpaya/Collections/BP_Charles` _returnvalue))
      (set `self.PlayerCharacter` _asbp_charles))))