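; Lightning ball VFX actor that throws jittering electric arcs onto surrounding geometry.
; On a Tick-driven cooldown, it line-traces in a random direction between two radii and spawns an attached Niagara arc on a hit, passing beam endpoints and impact normal.
; Optional secondary traces chain from each last impact, offset along its normal, within a cone around the primary direction, spawning secondary arcs until one misses.
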(event `self.ReceiveTick`
  (params (DeltaSeconds :type "Float (single-precision)"))
  (`self.UpdateTraces`))

(fn `UpdateTraces`
  (locals (RandomDirection :type "Vector Structure") (ImpactOffset :type "Float (double-precision)" :default 1.0) (LastHitLocation :type "Vector Structure") (LastHitWithOffset :type "Vector Structure") (LastHitNormal :type "Vector Structure"))
  (bind _returnvalue (`self.K2_GetActorLocation`))
  (bind _returnvalue_2 (* (`local.RandomDirection`) (`self.MinRadius`)))
  (bind _returnvalue_3 (+ (`local.LastHitLocation`) (* (`local.LastHitNormal`) (`self.SecondTraceOffset`))))
  ;[0 1 0.9559 0.33] Check CD
  (if (>= (- (`GameplayStatics.GetTimeSeconds`) (`self.LastTrace`)) (`self.TraceCooldown`))
    ;[0 1 0.9559 0.33] Line Trace
    (set `local.RandomDirection` (`KismetMathLibrary.RandomUnitVector`))
    (bind _outhit (`KismetSystemLibrary.LineTraceSingle` :`Start` (+ _returnvalue _returnvalue_2) :`End` (+ _returnvalue (* (`local.RandomDirection`) (`self.MaxRadius`))) :`TraceChannel` "TraceTypeQuery1" :`DrawTime` (`self.TraceCooldown`)))
    ;[0 1 0.9559 0.33] Reset CD
    (set `self.LastTrace` (`GameplayStatics.GetTimeSeconds`))
    (bind (_bblockinghit _binitialoverlap _time _distance _location _impactpoint _normal _impactnormal) (`GameplayStatics.BreakHitResult` _outhit))
    (if _bblockinghit
      (`|ExecutionSequence`
        (:`then_0`
          ;[0 1 0.9559 0.33] Spawn Electrics Arcs + Set Parameter's
          (bind _returnvalue_4 (`NiagaraFunctionLibrary.SpawnSystemAttached` "/Game/1_Art/VFX/NS_Lightning_Arcs_Jitter.NS_Lightning_Arcs_Jitter" (`self.LightningBall`) "None" (0.0 0.0 0.0) (struct) "KeepRelativeOffset" true))
          (`NiagaraComponent.SetVariableVec3` _returnvalue_4 "BeamStartPoint" _returnvalue_2)
          (bind _returnvalue_5 (+ _impactpoint (* _impactnormal (`local.ImpactOffset`))))
          (`NiagaraComponent.SetVariableVec3` _returnvalue_4 "BeamEndPoint" _returnvalue_5)
          (`NiagaraComponent.SetVariableVec3` _returnvalue_4 "ImpactNormal" _impactnormal)
          (set `local.LastHitLocation` _impactpoint)
          (set `local.LastHitWithOffset` _returnvalue_5)
          (set `local.LastHitNormal` _impactnormal))
        (:`then_1`
          (if (`self.IsSecondTraces`)
            (for _ (range (+ (`self.MaxSecondaryTraces`) 1))
              ;[0 1 0.9559 0.33] Secondary Traces
              ; HOW IT WORK :
              ; For the origin we're taking the last hit impact location and offset it by the direction of the normal.
              ; Then we're picking a new random direction in a cone aligned with the previous one and project that from the origin
              (bind _outhit_2 (`KismetSystemLibrary.LineTraceSingle` :`Start` _returnvalue_3 :`End` (+ _returnvalue_3 (* (`KismetMathLibrary.RandomUnitVectorInConeInDegrees` (`local.RandomDirection`) (`self.SecondaryTraceRandomDirection`)) (`self.MaxRadius`))) :`TraceChannel` "TraceTypeQuery1" :`DrawTime` 1.0))
              (bind (_bblockinghit_2 _binitialoverlap_2 _time_2 _distance_2 _location_2 _impactpoint_2 _normal_2 _impactnormal_2) (`GameplayStatics.BreakHitResult` _outhit_2))
              (if _bblockinghit_2
                (bind _returnvalue_6 (`NiagaraFunctionLibrary.SpawnSystemAttached` "/Game/1_Art/VFX/NS_Lightning_Arcs_Jitter_Secondary.NS_Lightning_Arcs_Jitter_Secondary" (`self.LightningBall`) "None" (0.0 0.0 0.0) (struct) "KeepRelativeOffset" true))
                (`NiagaraComponent.SetVariableVec3` _returnvalue_6 "BeamStartPoint" (`local.LastHitWithOffset`))
                (bind _returnvalue_7 (+ _impactpoint_2 (* _impactnormal_2 (`local.ImpactOffset`))))
                (`NiagaraComponent.SetVariableVec3` _returnvalue_6 "BeamEndPoint" _returnvalue_7)
                (`NiagaraComponent.SetVariableVec3` _returnvalue_6 "ImpactNormal" _impactnormal_2)
                (set `local.LastHitLocation` _impactpoint_2)
                (set `local.LastHitWithOffset` _returnvalue_7)
                (set `local.LastHitNormal` _impactnormal_2)
                (else
                  (break))))))))))

(fn `UserConstructionScript`)