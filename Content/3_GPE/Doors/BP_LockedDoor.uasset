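; Locked door GPE whose door component slides vertically or horizontally when the UnlockGPE event fires.
; The construction script places it at DoorClosedPosition or, in the Opened state, offsets it by its bounds size along the DoorOpenType axis.
; On unlock, a timeline lerps it from its BeginPlay position to DoorClosedPosition on that axis, so only a door starting Opened is displaced by the animation.
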(event `self.ReceiveBeginPlay`
  (`parent.ReceiveBeginPlay`)
  (set `self.InitialOffset` (`SceneComponent.RelativeLocation` (`self.Door`))))

(event `self.UnlockGPE`
  (params (DamageContext :type "/Game/0_Design/LifeSystem/Structs/F_DamageContext Structure"))
  (bind (_direction _smoothopen) (`Timeline|Timeline` :!via `PlayFromStart`)
    (:`Update`
      (set `self.Smooth Open` _smoothopen)
      (switch `/Game/3_GPE/Doors/E_DoorOpenType` (`self.DoorOpenType`)
        (:`NewEnumerator0`
          (`self.OpenVerticaly` :!label _label))
        (:`NewEnumerator3`
          (goto _label))
        (:`NewEnumerator1`
          (`self.OpenHorizontaly` :!label _label_2))
        (:`NewEnumerator2`
          (goto _label_2))))))

(fn `OpenHorizontaly`
  (bind _doorclosedposition_x (`KismetMathLibrary.BreakVector` (`self.DoorClosedPosition`)))
  (bind (_initialoffset_x _initialoffset_y _initialoffset_z) (`KismetMathLibrary.BreakVector` (`self.InitialOffset`)))
  (`SceneComponent.K2_SetRelativeLocation` (`self.Door`) (`KismetMathLibrary.MakeVector` (`KismetMathLibrary.Lerp` _initialoffset_x _doorclosedposition_x (`self.Smooth Open`)) _initialoffset_y _initialoffset_z) false false))

(fn `OpenVerticaly`
  (bind (_doorclosedposition_x _doorclosedposition_y _doorclosedposition_z) (`KismetMathLibrary.BreakVector` (`self.DoorClosedPosition`)))
  (bind (_initialoffset_x _initialoffset_y _initialoffset_z) (`KismetMathLibrary.BreakVector` (`self.InitialOffset`)))
  (`SceneComponent.K2_SetRelativeLocation` (`self.Door`) (`KismetMathLibrary.MakeVector` _initialoffset_x _initialoffset_y (`KismetMathLibrary.Lerp` _initialoffset_z _doorclosedposition_z (`self.Smooth Open`))) false false))

(fn `UserConstructionScript`
  (locals (DoorLocation :type "Vector Structure" :default (0.0 0.0 0.0)))
  (bind (_doorextent_x _doorextent_y _doorextent_z) (`KismetMathLibrary.BreakVector` (`self.DoorExtent`)))
  (bind (_doorextent_x_2 _doorextent_y_2 _doorextent_z_2) (`KismetMathLibrary.BreakVector` (`self.DoorExtent`)))
  (bind _doorextent_x_3 (`KismetMathLibrary.BreakVector` (`self.DoorExtent`)))
  (bind _doorextent_x_4 (`KismetMathLibrary.BreakVector` (`self.DoorExtent`)))
  (`parent.UserConstructionScript`)
  (set `self.DoorExtent` (* (`.BoxExtent` (`KismetSystemLibrary.GetComponentBounds` (`self.Door`))) 2.0))
  (switch `/Game/3_GPE/Doors/E_DoorState` (`self.DoorState`)
    (:`NewEnumerator1`
      (set `local.DoorLocation` (`self.DoorClosedPosition`)))
    (:`NewEnumerator0`
      (switch `/Game/3_GPE/Doors/E_DoorOpenType` (`self.DoorOpenType`)
        (:`NewEnumerator0`
          (set `local.DoorLocation` (+ (`self.DoorClosedPosition`) (`KismetMathLibrary.MakeVector` 0.0 0.0 _doorextent_z))))
        (:`NewEnumerator3`
          (set `local.DoorLocation` (+ (`self.DoorClosedPosition`) (`KismetMathLibrary.MakeVector` 0.0 0.0 (* _doorextent_z_2 -1.0)))))
        (:`NewEnumerator1`
          (set `local.DoorLocation` (+ (`self.DoorClosedPosition`) (`KismetMathLibrary.MakeVector` (* _doorextent_x_3 -1.0)))))
        (:`NewEnumerator2`
          (set `local.DoorLocation` (+ (`self.DoorClosedPosition`) (`KismetMathLibrary.MakeVector` _doorextent_x_4)))))))
  (`SceneComponent.K2_SetRelativeLocation` (`self.Door`) (`local.DoorLocation`) false false))