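; BP_CircuitBreaker is a one-shot interactable breaker that fires linked trigger receivers when used or destroyed.
; On BeginPlay it caches its BP_TriggerEventReceiver components.
; Both interaction and life component death call OnTriggerBoxEnter on each receiver, then disable the interaction collisions and destroy the interaction components and widget.
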(event `self.ReceiveBeginPlay`
  (`parent.ReceiveBeginPlay`)
  (set `self.MyTriggerComponents` (`self.K2_GetComponentsByClass` "/Game/Design/EnvironmentEvents/Components/BP_TriggerEventReceiver_Component.BP_TriggerEventReceiver_Component_C")))

(event `self.InteractableComponent.OnInteract`
  (for _array_element (`self.MyTriggerComponents`) :!label _label
    (`/Game/Design/EnvironmentEvents/Components/BP_TriggerEventReceiver_Component.OnTriggerBoxEnter` _array_element self))
  (`PrimitiveComponent.SetCollisionEnabled` (`self.OutterInteraction`) "NoCollision")
  (`PrimitiveComponent.SetCollisionEnabled` (`self.InnerInteraction`) "NoCollision")
  (`ActorComponent.K2_DestroyComponent` (`self.InteractableComponent`))
  (`ActorComponent.K2_DestroyComponent` (`self.Widget`))
  (`ActorComponent.K2_DestroyComponent` (`self.OutterInteraction`))
  (`ActorComponent.K2_DestroyComponent` (`self.InnerInteraction`)))

(event `self.BP_LifeComponent.OnDeath`
  (params (DamageContext :type "/Game/Design/LifeSystem/Structs/F_DamageContext Structure"))
  (goto _label))

(fn `UserConstructionScript`
  (`parent.UserConstructionScript`))