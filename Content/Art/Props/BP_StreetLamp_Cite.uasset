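; Street lamp prop whose spot light goes out once all of its destructible bulbs are destroyed.
; On BeginPlay it scans its child actor components for BP_Destructible_LightBulbe actors, binds to each one's destroy event and counts them.
; Each bulb destruction decrements that count, and the SpotLight component is destroyed when it reaches zero.
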(event `self.ReceiveBeginPlay`
  (for _array_element (`self.K2_GetComponentsByClass` "/Script/Engine.ChildActorComponent")
    (bind _asbp_destructible_light_bulbe (cast `/Game/Design/GPE/Destructible/BP_Destructible_LightBulbe` (`ChildActorComponent.ChildActor` _array_element)))
    (add `/Game/Design/GPE/Destructible/BP_Destructible_LightBulbe.OnDestroy` _asbp_destructible_light_bulbe (delegate `OnBulbDestroyed`))
    (`/Engine/EditorBlueprintResources/StandardMacros.IncrementInt` (`self.LightBulbLeft`))))

(event `OnBulbDestroyed`
  (bind _result (`/Engine/EditorBlueprintResources/StandardMacros.DecrementInt` (`self.LightBulbLeft`))
    (:`  `
      (if (== _result 0)
        (`ActorComponent.K2_DestroyComponent` (`self.SpotLight`))))))

(fn `UserConstructionScript`)