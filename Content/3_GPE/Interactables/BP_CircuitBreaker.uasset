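; BP_CircuitBreaker is a one-shot interactable that fires its trigger receivers when the player uses it.
; On BeginPlay it caches all BP_TriggerEventReceiver_Component instances on itself.
; OnInteract calls OnTriggerBoxEnter on each with itself as argument, reusing the trigger-box event path for a manual interaction.
; It then disables collision on both interaction volumes and destroys them, the widget and the InteractableComponent, preventing reuse.
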(event `self.ReceiveBeginPlay`
  (`parent.ReceiveBeginPlay`)
  (set `self.MyTriggerComponents` (`self.K2_GetComponentsByClass` "/Game/0_Design/EnvironmentEvents/Components/BP_TriggerEventReceiver_Component.BP_TriggerEventReceiver_Component_C")))

(event `self.InteractableComponent.OnInteract`
  (for _array_element (`self.MyTriggerComponents`)
    (`/Game/0_Design/EnvironmentEvents/Components/BP_TriggerEventReceiver_Component.OnTriggerBoxEnter` _array_element self))
  (`PrimitiveComponent.SetCollisionEnabled` (`self.OutterInteraction`) "NoCollision")
  (`PrimitiveComponent.SetCollisionEnabled` (`self.InnerInteraction`) "NoCollision")
  (`ActorComponent.K2_DestroyComponent` (`self.InteractableComponent`))
  (`ActorComponent.K2_DestroyComponent` (`self.Widget`))
  (`ActorComponent.K2_DestroyComponent` (`self.OutterInteraction`))
  (`ActorComponent.K2_DestroyComponent` (`self.InnerInteraction`)))

(fn `UserConstructionScript`
  (`parent.UserConstructionScript`))