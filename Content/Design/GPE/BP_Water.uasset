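; Water volume gameplay element that conducts electricity to the pawns inside it.
; When an overlapping actor's ElectrocutableComponent starts, the water electrocutes itself through its own component, which toggles the electric FX.
; While electrified, each tick box-queries pawns in the collision bounds, applying Shock damage and electrocution at a timestamp-throttled rate.
; The construction script sizes both water and electric FX grids to the collision box.
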(event `self.ElectrocutableComponent.OnElectricStart`
  (params (Duration :type "Float (single-precision)"))
  (`ActorComponent.Activate` (`self.ElectricFX`) false))

(event `self.ElectrocutableComponent.OnElectricTick`
  (params (DeltaTime :type "Float (single-precision)"))
  (bind _returnvalue (`GameplayStatics.GetTimeSeconds`))
  (bind (_origin _boxextent) (`KismetSystemLibrary.GetComponentBounds` (`self.CollisionComponent`)))
  (bind _returnvalue_2 (<= (- (`self.NextDamageTime`) _returnvalue) 0.0))
  (bind _outactors (`KismetSystemLibrary.BoxOverlapActors` _origin _boxextent (`|MakeArray` "ObjectTypeQuery3" :!type "EObjectTypeQuery Enum")))
  (bind _output_get (set `self.OverlappedActors` _outactors))
  (for _array_element _output_get
    (if _returnvalue_2
      (bind _returnvalue_3 (`self.GetComponentByClass` _array_element "/Script/MetroXHunter.HealthComponent"))
      (`/Engine/EditorBlueprintResources/StandardMacros.IsValid` _returnvalue_3
        (:`Is Valid`
          (`HealthComponent.TakeDamage` _returnvalue_3 (make `DamageContext` (`self.DamagePerTick`) "Shock" self)))
        (:`Is Not Valid`
          _))
      (bind _returnvalue_4 (`self.GetComponentByClass` _array_element "/Script/MetroXHunter.ElectrocutableComponent"))
      (`/Engine/EditorBlueprintResources/StandardMacros.IsValid` _returnvalue_4
        (:`Is Valid`
          (`ElectrocutableComponent.Electrocute` _returnvalue_4 3.0)))))
  (if _returnvalue_2
    (set `self.NextDamageTime` (+ _returnvalue (/ 1.0 (`KismetMathLibrary.Conv_IntToDouble` (`self.DamageTickPerSeconds`)))))))

(event `self.ElectrocutableComponent.OnElectricEnd`
  (`ActorComponent.Deactivate` (`self.ElectricFX`)))

(event `self.ReceiveBeginPlay`)

(event `self.ReceiveActorBeginOverlap`
  (params (OtherActor :type "Actor Object Reference"))
  (bind _returnvalue (`self.GetComponentByClass` OtherActor "/Script/MetroXHunter.ElectrocutableComponent"))
  (`/Engine/EditorBlueprintResources/StandardMacros.IsValid` _returnvalue
    (:`Is Valid`
      (add `ElectrocutableComponent.OnElectricStart` _returnvalue (delegate `OnActorElectricStart`)))))

(event `OnActorElectricStart`
  (params (Duration :type "Float (single-precision)"))
  (bind _electrocutablecomponent (`self.ElectrocutableComponent`))
  ;[1 1 1 0.33] Electrocute water if one actor become electrocuted
  (if (not (`ElectrocutableComponent.IsElectrocuting` _electrocutablecomponent))
    (`ElectrocutableComponent.Electrocute` _electrocutablecomponent 5.0)))

(event `self.ReceiveActorEndOverlap`
  (params (OtherActor :type "Actor Object Reference"))
  (bind _returnvalue (`self.GetComponentByClass` OtherActor "/Script/MetroXHunter.ElectrocutableComponent"))
  (`/Engine/EditorBlueprintResources/StandardMacros.IsValid` _returnvalue
    (:`Is Valid`
      (remove `ElectrocutableComponent.OnElectricStart` _returnvalue (delegate `OnActorElectricStart`)))))

(fn `UserConstructionScript`
  (bind (_returnvalue_x _returnvalue_y) (`KismetMathLibrary.BreakVector` (`BoxComponent.GetScaledBoxExtent` (cast `BoxComponent` (`self.CollisionComponent`) :!pure true))))
  (bind _returnvalue (* _returnvalue_x 2.0))
  (bind _returnvalue_2 (* _returnvalue_y 2.0))
  (`NiagaraComponent.SetVariableVec2` (`self.WaterFX`) "WorldGridSize" (`KismetMathLibrary.MakeVector2D` _returnvalue _returnvalue_2))
  (`NiagaraComponent.SetVariableVec2` (`self.ElectricFX`) "Grid Size" (`KismetMathLibrary.MakeVector2D` _returnvalue _returnvalue_2))
  (`SceneComponent.SetHiddenInGame` (`self.SpriteComponent`) true false))