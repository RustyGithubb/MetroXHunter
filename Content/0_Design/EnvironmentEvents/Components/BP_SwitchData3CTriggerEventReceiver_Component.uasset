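; A trigger event receiver component that switches the player's 3C data when a trigger box event plays.
; On BeginPlay it caches the player pawn as a Character, printing a message if the cast fails.
; The component-specific event passes either the In or Out set of locomotion value, spring arm and locomotion behavior data to the character's BPAC_SwitchData3C component, depending on whether the box was entered.
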(event `self.ReceiveBeginPlay`
  ;[0 0 0] Cast Character
  (bind _ascharacter (cast `Character` (`GameplayStatics.GetPlayerPawn` 0))
    (:`then`
      (set `self.As Character` _ascharacter))
    (:`CastFailed`
      (`KismetSystemLibrary.PrintString` "// ------- Any character Detected " true true (struct :`R` 0.698145 :`B` 1.0 :`A` 1.0) 500.0))))

(fn `OnPlayComponentSpecificEvent`
  (params (FromBoxEnter :type Boolean) (TriggerBox :type "Actor Object Reference"))
  (bind _returnvalue (`Actor.GetComponentByClass` (`self.As Character`) "/TPS_FeedlingAddon/TPS/BPAC_SwitchData3C.BPAC_SwitchData3C_C"))
  (if FromBoxEnter
    (`/TPS_FeedlingAddon/TPS/BPAC_SwitchData3C.SwitchdataComponent` _returnvalue (`self.Data Locomotion Value_In`) (`self.Data Spring Arm_In`) (`self.Data Locomotion Behavior_In`))
    (else
      (`/TPS_FeedlingAddon/TPS/BPAC_SwitchData3C.SwitchdataComponent` _returnvalue (`self.Data Locomotion Value_Out`) (`self.Data Spring Arm_Out`) (`self.Data Locomotion Behavior_Out`)))))