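; Level-design trigger box that notifies receiver components on a linked actor when the main character enters or exits.
; BeginPlay caches the linked actor's BP_TriggerEventReceiver_Component instances, printing an error unless suppressed if none exist.
; Overlaps only fire when the player's event flags match NecessaryFlags, and one-time boxes destroy their components after a valid exit.
; The construction script drives a resizable, color-coded visualizer with a camera-aligned custom label, optionally hidden in game.
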(event `self.ReceiveBeginPlay`
  (`self.GetReceiverComponent`)
  ;[1 1 1 0.33] Should Show Ingame? (for debug purposes probably)
  (`SceneComponent.SetHiddenInGame` (`self.DONT_MOVE_TriggerBox`) (not (`self.ShowIngame`)) false)
  (`SceneComponent.SetHiddenInGame` (`self.TextRender`) (not (`self.ShowIngame`)) false)
  (`SceneComponent.SetHiddenInGame` (`self.VisualizerCube`) (not (`self.ShowIngame`)) false)
  ;[1 1 1 0.33] Cache Player FlagComponent if we need to check flags
  (if (`BlueprintMapLibrary.Map_IsNotEmpty` (`self.NecessaryFlags`))
    (set `self.CharacterFlagComponent` (`self.GetComponentByClass` (`GameplayStatics.GetPlayerPawn` 0) "/Game/0_Design/EnvironmentEvents/BP_EventFlagsComponent.BP_EventFlagsComponent_C"))))

(event `self.DONT_MOVE_TriggerBox.OnComponentBeginOverlap`
  (params (OverlappedComponent :type "PrimitiveComponent Object Reference") (OtherActor :type "Actor Object Reference") (OtherComp :type "PrimitiveComponent Object Reference") (OtherBodyIndex :type Integer) (bFromSweep :type Boolean) (SweepResult :type "HitResult Structure (by ref)"))
  (if (`/Game/o_Libraries/BPL_GeneralUtilities.Is Actor Of Class` OtherActor "/Game/0_Design/GameManagement_/BP_MainChara.BP_MainChara_C")
    (bind _everythingright (`self.AreFlagsCorrect`))
    (if _everythingright
      (for _array_element (`self.ComponentsToCall`)
        (`/Game/0_Design/EnvironmentEvents/Components/BP_TriggerEventReceiver_Component.OnTriggerBoxEnter` _array_element)))))

(event `self.DONT_MOVE_TriggerBox.OnComponentEndOverlap`
  (params (OverlappedComponent :type "PrimitiveComponent Object Reference") (OtherActor :type "Actor Object Reference") (OtherComp :type "PrimitiveComponent Object Reference") (OtherBodyIndex :type Integer))
  (if (`/Game/o_Libraries/BPL_GeneralUtilities.Is Actor Of Class` OtherActor "/Game/0_Design/GameManagement_/BP_MainChara.BP_MainChara_C")
    (bind _everythingright (`self.AreFlagsCorrect`))
    (if _everythingright
      (for _array_element (`self.ComponentsToCall`)
        (`/Game/0_Design/EnvironmentEvents/Components/BP_TriggerEventReceiver_Component.OnTriggerBoxExit` _array_element))
      ;[1 0.4063 0.3165 0.33] Should Destroy after One-Time Use?
      (if (`self.OneTimeUse`)
        (`ActorComponent.K2_DestroyComponent` (`self.DONT_MOVE_TriggerBox`))
        (`ActorComponent.K2_DestroyComponent` (`self.TextRender`))
        (`ActorComponent.K2_DestroyComponent` (`self.VisualizerCube`))))))

(fn `AreFlagsCorrect`
  (returns (EverythingRight :type Boolean))
  (locals (Keys :type "Array of GameplayTag Structure") (Values :type "Array of Boolean") (isRight :type Boolean))
  (`self.CharacterFlagComponent`
    (:`then`
      (`|ExecutionSequence`
        (:`then_0`
          ;[1 1 1 0.33] Caching
          (bind _keys (`BlueprintMapLibrary.Map_Keys` (`self.NecessaryFlags`)))
          (set `local.Keys` _keys)
          (bind _values (`BlueprintMapLibrary.Map_Values` (`self.NecessaryFlags`)))
          (set `local.Values` _values)
          (set `local.isRight` true))
        (:`then_1`
          (for (_array_element _array_index) (`local.Keys`)
            (bind _flagvalue (`/Game/0_Design/EnvironmentEvents/BP_EventFlagsComponent.GetFlagValue` (`self.CharacterFlagComponent`) _array_element))
            (if (not (== _flagvalue (`|GetArrayItem` (`local.Values`) _array_index)))
              (set `local.isRight` false)
              (break)))
          (return (`local.isRight`)))))
    (:`else`
      ;[1 1 1 0.33] No flags to check?
      ; Good to go!
      (return true))))

(fn `GetReceiverComponent`
  ;[0.04963 0.5881 1 0.33] Is this Box connected to an Actor? That has at least one ReceiverComponent?
  (bind _linkedreceiveractor (`self.LinkedReceiverActor`)
    (:`then`
      (`/Engine/EditorBlueprintResources/StandardMacros.IsValid` (`self.GetComponentByClass` _linkedreceiveractor "/Game/0_Design/EnvironmentEvents/Components/BP_TriggerEventReceiver_Component.BP_TriggerEventReceiver_Component_C")
        (:`Is Valid`
          ;[0.8048 0.4297 1 0.33] If yes save all Components
          (set `self.ComponentsToCall` (`self.K2_GetComponentsByClass` (`self.LinkedReceiverActor`) "/Game/0_Design/EnvironmentEvents/Components/BP_TriggerEventReceiver_Component.BP_TriggerEventReceiver_Component_C")))
        (:`Is Not Valid`
          ;[0.4676 1 0.4728 0.33] Else Print Error
          (if (not (`self.DontPrintError`)) :!label _label
            (`KismetSystemLibrary.PrintText` (`|FormatText` "TriggerBoxEvent with name {name} isn't linked to an Actor, or is linked to an Actor not possessing a BP_TriggerEventReceiver_Component inheriting component. \nPlease set \"LinkedReceiverActor\" to an Actor with an ActorComponent inheriting from BP_TriggerEventReceiver_Component. \nElse, check the \"Don't Print Error\" on the TriggerBox" (`KismetSystemLibrary.GetDisplayName` self)) true true (struct :`R` 1.0 :`A` 1.0) 5000.0)))))
    (:`else`
      (goto _label))))

(fn `UserConstructionScript`
  (bind (_boxsizehandle_x _boxsizehandle_y) (`KismetMathLibrary.BreakVector` (`self.BoxSizeHandle`)))
  (`self.TextMaterial`
    (:`then`
      _)
    (:`else`
      (bind _returnvalue (`PrimitiveComponent.CreateDynamicMaterialInstance` (`self.TextRender`) 0 "/Game/1_Art/MaterialLibrary/DebugMaterials/M_CameraAlignedText.M_CameraAlignedText" "None"))
      (set `self.TextMaterial` _returnvalue)))
  ;[0 0 0 0.33] Set the correct size for the Trigger Box, the "OneTimeUse" visualizer box, and the Text inside (so it doesn't get too long)
  (`SceneComponent.K2_SetRelativeLocation` (`self.DONT_MOVE_TriggerBox`) (0.0 0.0 0.0) false false)
  (`BoxComponent.SetBoxExtent` (`self.DONT_MOVE_TriggerBox`) (`self.BoxSizeHandle`) false)
  (`SceneComponent.SetRelativeScale3D` (`self.VisualizerCube`) (* (`self.BoxSizeHandle`) 0.02))
  (`TextRenderComponent.SetWorldSize` (`self.TextRender`) (* (`KismetMathLibrary.FMax` (`KismetMathLibrary.Abs` _boxsizehandle_x) (`KismetMathLibrary.Abs` _boxsizehandle_y)) 0.2 (`self.TextScaleMultiplier`)))
  ;[0 0 0 0.33] Red if the TriggerBox is one-time-use
  ; Blue otherwise
  (`PrimitiveComponent.SetMaterial` (`self.VisualizerCube`) 0 (select `bool` (`self.OneTimeUse`) :`false` "/Game/1_Art/MaterialLibrary/DebugMaterials/Instances/MI_TranslucentBlue.MI_TranslucentBlue" :`true` "/Game/1_Art/MaterialLibrary/DebugMaterials/Instances/MI_TranslucentRed.MI_TranslucentRed" :!type "MaterialInterface Object Reference"))
  ;[0 0 0 0.33] Set a custom visible name.
  ; I could use the "FitTextToNumberOfCharacters" but with the camera-oriented text and many different sizes possible for the TriggerBox, the LD is better of making line breaks themselves...
  (`TextRenderComponent.K2_SetText` (`self.TextRender`) (`self.TriggerCustomName`))
  ;[0 0 0 0.33] TextColor & Emissive
  (`TextRenderComponent.SetTextRenderColor` (`self.TextRender`) (`KismetMathLibrary.Conv_LinearColorToColor` (`self.TextColor`)))
  (`MaterialInstanceDynamic.SetScalarParameterValue` (`self.TextMaterial`) "TextEmissive" (`self.TextEmissiveIntensity`)))