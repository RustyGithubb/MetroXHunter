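; Cheat function that switches the player character's reload system to one of several configurable classes.
; On init it sets the value range from the class list and caches the controlled BP_MainChara pawn after a one-tick delay.
; On activation it uses the truncated cheat value as an index, has the character create that reload system, and prints the chosen class name on screen.
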(event `self.OnInit`
  (set `self.MaxValue` (`KismetMathLibrary.Conv_IntToDouble` (- (`KismetArrayLibrary.Array_Length` (`self.ReloadSystemClasses`)) 1)))
  (`KismetSystemLibrary.DelayUntilNextTick`)
  (bind _asbp_main_chara (cast `/Game/0_Design/GameManagement_/BP_MainChara` (`Controller.K2_GetPawn` (`CheatManager.GetPlayerController` (`self.CheatManager`)))))
  (set `self.PlayerCharacter` _asbp_main_chara))

(event `self.OnCheat`
  (bind _output (`|GetArrayItem` (`self.ReloadSystemClasses`) (`KismetMathLibrary.FTrunc` (`self.Value`))))
  (`/Game/0_Design/GameManagement_/BP_MainChara.CreateReloadSystem` (`self.PlayerCharacter`) _output)
  (`KismetSystemLibrary.PrintText` (`|FormatText` "Cheat: Switching to Reload System '{Name}'" (`KismetSystemLibrary.GetClassDisplayName` _output)) true true (struct :`G` 0.66 :`B` 1.0 :`A` 1.0) 5.0))