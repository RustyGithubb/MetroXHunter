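; Acid projectile for an enemy, using big monster impact audio, that handles the effects when it explodes.
; On explosion it disables collision, deactivates the acid effect and spawns an impact Niagara system oriented from the hit normal.
; A short trace against that normal places an acid pool on the surface.
; Audio fades out as an impact sound plays, and a short lifespan covers the fade before destruction.
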(event `self.OnExploded`
  (params (HitResult :type "HitResult Structure (by ref)"))
  (bind _returnvalue (`self.K2_GetActorLocation`))
  (bind _audio (`self.Audio`))
  (`self.SetActorEnableCollision` false)
  (`ActorComponent.Deactivate` (`self.Acid`))
  (`NiagaraFunctionLibrary.SpawnSystemAtLocation` "/Game/Art/VFX/NS_Acid/NS_Acid_Impact.NS_Acid_Impact" (`self.K2_GetActorLocation`) (`KismetMathLibrary.Conv_VectorToRotator` (`KismetMathLibrary.Cross_VectorVector` HitResult_ImpactNormal (`KismetMathLibrary.Vector_Right`))) (1.0 1.0 1.0) true true "AutoRelease")
  (`KismetSystemLibrary.LineTraceSingle` (0.0 0.0 0.0) (0.0 0.0 0.0) "TraceTypeQuery1")
  (bind _outhit (`KismetSystemLibrary.LineTraceSingle` _returnvalue (+ _returnvalue (* (`KismetMathLibrary.NegateVector` HitResult_ImpactNormal) 160.0)) "TraceTypeQuery1"))
  (bind (_bblockinghit _binitialoverlap _time _distance _location _impactpoint _normal) (`GameplayStatics.BreakHitResult` _outhit))
  (`NiagaraFunctionLibrary.SpawnSystemAtLocation` "/Game/Art/VFX/NS_Acid/NS_Acid_Pool_V1.NS_Acid_Pool_V1" _location (`KismetMathLibrary.Conv_VectorToRotator` _normal) (1.0 1.0 1.0) true true "AutoRelease")
  ;[0 0.6886 1 0.33] SOUND
  (`AudioComponent.FadeOut` _audio 0.5 0.0 "Linear")
  (`GameplayStatics.PlaySoundAtLocation` "/Game/Sounds/Audio/SD/SoundWaves/Enemies/BigMonster/Acide/SW_SFX_BigMonster_AcidImpact.SW_SFX_BigMonster_AcidImpact" (`SceneComponent.K2_GetComponentLocation` _audio) (struct) 1.0 1.0 0.0 (`AudioComponent.AttenuationSettings` _audio) null null null)
  (`self.SetLifeSpan` 1.0) ; The lifespan must encapsulate the audio's fading out time
)

(fn `UserConstructionScript`)