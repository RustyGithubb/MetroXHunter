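; Sound manager component for the Springfield gun, handling audio for both its rifle and lightning (Tesla) modes.
; Rifle events spawn one-shots on the Bobine's audio component, varying shots by remaining ammo, plus shell drops and delayed surface-based impacts pulled back to avoid occlusion.
; Lightning mode plays a looping sound on that component, driven by trigger parameters for its states.
; Tick, enabled only while lightning is active, feeds it the normalized energy level.
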(event `self.ReceiveBeginPlay`
  (`KismetSystemLibrary.DelayUntilNextTick`)
  ;[1 1 1 0.33] Retrieve Audio Component attached to the springfield
  (bind _output_get (set `self.Springfield` (cast `/Game/Developers/corentinpaya/Collections/BP_Springfield` (`self.GetOwner`) :!pure true)))
  (set `self.MuzzleAudioComponent` (`/Game/Developers/corentinpaya/Collections/BP_Springfield.LightningAudio` _output_get))
  ;[1 1 1 0.33] Retrieve Audio Component attached on Bobine
  (set `self.BobineAudioComponent` (`/Game/Design/_GameManagement/BP_Bobine.Audio` (cast `/Game/Design/_GameManagement/BP_Bobine` (`MetroPlayerCharacter.Bobine` (`Gun.PlayerCharacter` (`self.Springfield`))) :!pure true)))
  ;[1 1 1 0.33] Bind to Reload
  (add `ReloadComponent.OnReloadStateChanged` (`Gun.ReloadComponent` (`self.Springfield`)) (`|CreateDelegate` :!event `OnRifleReloadStateChanged`)))

(event `self.OnRifleShoot`
  (params (HitResult :type "HitResult Structure (by ref)"))
  (bind (_bblockinghit _binitialoverlap _time _distance _location _impactpoint _normal _impactnormal _physmat _hitactor _hitcomponent _hitbonename _bonename _hititem _elementindex _faceindex _tracestart _traceend) (`GameplayStatics.BreakHitResult` HitResult))
  (bind _returnvalue (- _location (* (`KismetMathLibrary.GetDirectionUnitVector` _tracestart _traceend) 50.0)))
  ;[1 0.5073 0 0.33 32] RIFLE
  ;;[1 1 1 0.33] Play shoot sound
  (`GameplayStatics.SpawnSoundAttached` (select `int` (`KismetMathLibrary.Min` (`ReloadComponent.CurrentAmmoInMagazine` (`Gun.ReloadComponent` (`self.Springfield`))) 2) :`0` "/Game/Sounds/Audio/SD/MetaSounds/MS_Sources/MC/Weapon/Mosin/MS_Mosin_LastShot.MS_Mosin_LastShot" :`1` "/Game/Sounds/Audio/SD/MetaSounds/MS_Sources/MC/Weapon/Mosin/MS_Mosin_BeforeLastShot.MS_Mosin_BeforeLastShot" :`2` "/Game/Sounds/Audio/SD/MetaSounds/MS_Sources/MC/Weapon/Mosin/MS_Mosin_Shot.MS_Mosin_Shot" :!type "SoundBase Object Reference") (`self.BobineAudioComponent`) "None" (0.0 0.0 0.0) (struct) "KeepRelativeOffset" false 1.0 1.0 0.0 null null)
  ;;[1 1 1 0.33] Play impact sound depending on surface
  (`/Engine/EditorBlueprintResources/StandardMacros.IsValid` _physmat
    (:`Is Valid`
      (`KismetSystemLibrary.Delay` 0.1)
      (switch `EPhysicalSurface` (`PhysicalMaterial.SurfaceType` _physmat)
        (:`SurfaceType_Default`
          (`GameplayStatics.PlaySoundAtLocation` "/Game/Sounds/Audio/SD/MetaSounds/MS_Sources/MC/Weapon/Mosin/MS_BulletImpact_Concrete.MS_BulletImpact_Concrete" _returnvalue (struct) 1.0 1.0 0.0 null null null null :!label _label))
        (:`SurfaceType2`
          (goto _label))
        (:`SurfaceType4`
          (`GameplayStatics.PlaySoundAtLocation` "/Game/Sounds/Audio/SD/MetaSounds/MS_Sources/MC/Weapon/Mosin/MS_BulletImpact_Metal.MS_BulletImpact_Metal" _returnvalue (struct) 1.0 1.0 0.0 null null null null))
        (:`SurfaceType5`
          (`GameplayStatics.PlaySoundAtLocation` "/Game/Sounds/Audio/SD/MetaSounds/MS_Sources/MC/Weapon/Mosin/MS_BulletImpact_Lock.MS_BulletImpact_Lock" _returnvalue (struct) 1.0 1.0 0.0 null null null null))
        (:`SurfaceType6`
          (`GameplayStatics.PlaySoundAtLocation` "/Game/Sounds/Audio/SD/MetaSounds/MS_Sources/MC/Weapon/Mosin/MS_BulletImpact_Wood.MS_BulletImpact_Wood" _returnvalue (struct) 1.0 1.0 0.0 null null null null))
        (:`SurfaceType7`
          (`GameplayStatics.PlaySoundAtLocation` "/Game/Sounds/Audio/SD/MetaSounds/MS_Sources/MC/Weapon/Mosin/MS_BulletImpact_Organic.MS_BulletImpact_Organic" _returnvalue (struct) 1.0 1.0 0.0 null null null null))
        (:`SurfaceType8`
          (`GameplayStatics.PlaySoundAtLocation` "/Game/Sounds/Audio/SD/MetaSounds/MS_Sources/MC/Weapon/Mosin/MS_BulletImpact_Glass.MS_BulletImpact_Glass" _returnvalue (struct) 1.0 1.0 0.0 null null null null))))))

(event `self.OnRifleShootEmpty`
  ;[1 0.5073 0 0.33 32] RIFLE
  (`GameplayStatics.SpawnSoundAttached` "/Game/Sounds/Audio/SD/MetaSounds/MS_Sources/MC/Weapon/Mosin/MS_Mosin_Empty.MS_Mosin_Empty" (`self.BobineAudioComponent`) "None" (0.0 0.0 0.0) (struct) "KeepRelativeOffset" false 1.0 1.0 0.0 null null))

(event `self.OnRifleShellCollide`
  (params (ShellActor :type "Actor Object Reference") (bIsFirstCollision :type Boolean))
  ;[1 0.5073 0 0.33 32] RIFLE
  (if bIsFirstCollision
    (`GameplayStatics.PlaySoundAtLocation` "/Game/Sounds/Audio/SD/MetaSounds/MS_Sources/MC/Weapon/Mosin/MS_Mosin_Bulletdrops.MS_Mosin_Bulletdrops" (`Actor.K2_GetActorLocation` ShellActor) (struct) 1.0 1.0 0.0 null null null null)))

(event `self.OnRifleCocking`
  ;[1 0.5073 0 0.33 32] RIFLE
  (`GameplayStatics.SpawnSoundAttached` "/Game/Sounds/Audio/SD/MetaSounds/MS_Sources/MC/Weapon/Mosin/MS_Mosin_Reload.MS_Mosin_Reload" (`self.BobineAudioComponent`) "None" (0.0 0.0 0.0) (struct) "KeepRelativeOffset" false 1.0 1.0 0.0 null null))

(event `OnRifleReloadStateChanged`
  (params (ReloadState :type "EReloadState Enum" :default "Start"))
  ;[1 0.5073 0 0.33 32] RIFLE
  (switch `EReloadState` ReloadState
    (:`Normal`
      _)
    (:`Perfect`
      _))
  (`GameplayStatics.SpawnSoundAttached` "/Game/Sounds/Audio/SD/MetaSounds/MS_Sources/MC/Weapon/Mosin/MS_Mosin_Reload_Full.MS_Mosin_Reload_Full" (`self.BobineAudioComponent`) "None" (0.0 0.0 0.0) (struct) "KeepRelativeOffset" false 1.0 1.0 0.0 null null))

(event `self.OnLightningSwitch`
  (params (bIsLightningActive :type Boolean))
  ;[0 0.757 1 0.33 32] LIGHTNING
  (`GameplayStatics.SpawnSoundAttached` (select `bool` bIsLightningActive :`false` "/Game/Sounds/Audio/SD/MetaSounds/MS_Sources/MC/Weapon/TeslaGun/MS_TeslaGun_SwitchOff.MS_TeslaGun_SwitchOff" :`true` "/Game/Sounds/Audio/SD/MetaSounds/MS_Sources/MC/Weapon/TeslaGun/MS_TeslaGun_SwitchOn.MS_TeslaGun_SwitchOn" :!type "SoundBase Object Reference") (`self.BobineAudioComponent`) "None" (0.0 0.0 0.0) (struct) "KeepRelativeOffset" false 1.0 1.0 0.0 null null)
  (if bIsLightningActive
    (`self.OnLightningStartIdle`)
    (else
      (`self.OnLightningStopIdle`))))

(event `OnLightningStartIdle`
  (bind _bobineaudiocomponent (`self.BobineAudioComponent`))
  ;[0 0.757 1 0.33 32] LIGHTNING
  (`AudioComponent.SetSound` _bobineaudiocomponent "/Game/Sounds/Audio/SD/MetaSounds/MS_Sources/MC/Weapon/TeslaGun/MS_TeslaGunFull.MS_TeslaGunFull") ; NOTE: The sound asset must have "Looping" set to true
  (`AudioComponent.Play` _bobineaudiocomponent 0.0)
  (`self.SetComponentTickEnabled` true))

(event `OnLightningStopIdle`
  ;[0 0.757 1 0.33 32] LIGHTNING
  (`AudioParameterControllerInterface.SetTriggerParameter` (`self.BobineAudioComponent`) "TeslaOff")
  (`self.SetComponentTickEnabled` false))

(event `self.OnLightningStartCharging`
  ;[0 0.757 1 0.33 32] LIGHTNING
  (`AudioParameterControllerInterface.SetTriggerParameter` (`self.BobineAudioComponent`) "TeslaShooting"))

(event `self.OnLightningStopCharging`
  ;[0 0.757 1 0.33 32] LIGHTNING
  (`AudioParameterControllerInterface.SetTriggerParameter` (`self.BobineAudioComponent`) "TeslaStopShooting" :!label _label_2))

(event `self.ReceiveTick`
  (params (DeltaSeconds :type "Float (single-precision)"))
  ;[0 0.757 1 0.33 32] LIGHTNING
  (bind _springfield (`self.Springfield`)
    (:`then`
      (`AudioParameterControllerInterface.SetFloatParameter` (`self.BobineAudioComponent`) "EnergyAmount" (/ (`BaseGun.CurrentEnergyAmount` _springfield) (`GunData.MaxEnergyAmount` (`BaseGun.GunData` _springfield)))))
    (:`else`)))

(event `self.OnLightningStartShoot`
  ;[0 0.757 1 0.33 32] LIGHTNING
)

(event `self.OnLightningStopShoot`
  ;[0 0.757 1 0.33 32] LIGHTNING
  (goto _label_2))

(event `self.OnLightningShootEmpty`
  ;[0 0.757 1 0.33 32] LIGHTNING
  (`AudioParameterControllerInterface.SetTriggerParameter` (`self.BobineAudioComponent`) "TeslaEmpty"))

(event `self.OnLightningStartReload`
  ;[0 0.757 1 0.33 32] LIGHTNING
)

(event `self.OnLightningStopReload`
  ;[0 0.757 1 0.33 32] LIGHTNING
  (`AudioParameterControllerInterface.SetTriggerParameter` (`self.BobineAudioComponent`) "TeslaStopReload"))