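; BP_Desk is an interactable desk with a small metal drawer that opens and closes on interaction.
; The InteractableComponent's OnInteract drives a FlipFlop that plays or reverses a Timeline, lerping the StaticMesh's relative location along Y.
; Each direction spawns its own attached drawer sound.
; Interaction freezes when opening starts and unfreezes when the Timeline finishes; closing does not set the freeze.
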(event `self.InteractableComponent.OnInteract`
  (`/Engine/EditorBlueprintResources/StandardMacros.FlipFlop`
    (:`A`
      (`self.SetInteractionFreezed` true)
      (`GameplayStatics.SpawnSoundAttached` "/Game/Sounds/Audio/SD/SoundWaves/GPE/Locker/SW_GPE_LittleMetalDrawer_Open.SW_GPE_LittleMetalDrawer_Open" (`self.Desk`) "None" (0.0 0.0 0.0) (struct) "KeepRelativeOffset" false 1.0 1.0 0.0 null null)
      (bind (_direction _lerp) (`Timeline|Timeline` :!label _label)
        (:`Update`
          (`SceneComponent.K2_SetRelativeLocation` (`self.StaticMesh`) (`KismetMathLibrary.VLerp` (0.0 0.0 0.0) (0.0 36.0 0.0) _lerp) false false))
        (:`Finished`
          (`self.SetInteractionFreezed` false))))
    (:`B`
      (`GameplayStatics.SpawnSoundAttached` "/Game/Sounds/Audio/SD/SoundWaves/GPE/Locker/SW_GPE_LittleMetalDrawer_Close.SW_GPE_LittleMetalDrawer_Close" (`self.Desk`) "None" (0.0 0.0 0.0) (struct) "KeepRelativeOffset" false 1.0 1.0 0.0 null null)
      (goto _label :!via `Reverse`))))

(fn `UserConstructionScript`)