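; Cheat function that switches the player pawn's aim assist component on or off.
; On init it waits a tick, then caches the component and the sibling Difficulty and Aim Assist Debug cheat functions.
; Disabling also fires the debug cheat if it is togglable.
; A conditional macro checks the Difficulty cheat's current index to keep that selection in sync with the aim assist state.
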(event `self.OnInit`
  (`KismetSystemLibrary.DelayUntilNextTick`)
  (`self.GetReferences`))

(event `self.OnCheat`
  (bind _index (`MXHCheatSelectionFunction.Index` (`self.DifficultyCheatFunction`)))
  (switch `int` (`self.Index`)
    (:`0`
      (`self.DisableAimAssist`)
      (if (!= _index 2)
        (set `MXHCheatSelectionFunction.Index` 3 (`self.DifficultyCheatFunction`) :!label _label)))
    (:`1`
      (set `/AdvancedAimAssist/Blueprints/Components/AAA_BP_AimAssistComponent.bIsComponentEnable` true (`self.AimAssistComponent`))
      (if (not (< _index 2))
        (goto _label)))))

(fn `DisableAimAssist`
  (bind _aimassistdebugcheatfunction (`self.AimAssistDebugCheatFunction`))
  (`|ExecutionSequence`
    (:`then_0`
      (if (`MXHCheatFunction.bIsTogglable` _aimassistdebugcheatfunction)
        (`self.Cheat` :`self` _aimassistdebugcheatfunction)))
    (:`then_1`
      (set `/AdvancedAimAssist/Blueprints/Components/AAA_BP_AimAssistComponent.bIsComponentEnable` false (`self.AimAssistComponent`))
      (if (!= (`self.Index`) 0)
        (set `self.Index` 0)))))

(fn `GetReferences`
  (bind _returnvalue (`Controller.K2_GetPawn` (`CheatManager.GetPlayerController` (`self.CheatManager`))))
  (`/Engine/EditorBlueprintResources/StandardMacros.IsValid` _returnvalue
    (:`Is Valid`
      (set `self.AimAssistComponent` (`Actor.GetComponentByClass` _returnvalue "/AdvancedAimAssist/Blueprints/Components/AAA_BP_AimAssistComponent.AAA_BP_AimAssistComponent_C"))
      (`|ExecutionSequence`
        (:`then_0`
          (bind _returnvalue_2 (`MXHCheatManager.FindCheatFunctionOfClass` (`self.CheatManager`) "/Game/0_Design/CheatFunctions/BP_CheatFunction_Difficulty.BP_CheatFunction_Difficulty_C"))
          (bind _asbp_cheat_function_difficulty (cast `/Game/0_Design/CheatFunctions/BP_CheatFunction_Difficulty` _returnvalue_2))
          (set `self.DifficultyCheatFunction` _asbp_cheat_function_difficulty))
        (:`then_1`
          (bind _returnvalue_3 (`MXHCheatManager.FindCheatFunctionOfClass` (`self.CheatManager`) "/Game/0_Design/CheatFunctions/BP_CheatFunction_AimAssist_Debug.BP_CheatFunction_AimAssist_Debug_C"))
          (bind _asbp_cheat_function_aim_assist_debug (cast `/Game/0_Design/CheatFunctions/BP_CheatFunction_AimAssist_Debug` _returnvalue_3))
          (set `self.AimAssistDebugCheatFunction` _asbp_cheat_function_aim_assist_debug))))))