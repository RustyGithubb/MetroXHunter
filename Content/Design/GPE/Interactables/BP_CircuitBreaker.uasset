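; Circuit breaker interactable that only takes Shock damage to power up linked lighting and cables.
; Each shock activates cable lightning, starts a short or long area flicker sequence by remaining health, and fires a gameplay event once.
; Health regenerates on Tick.
; Flicker callbacks drive lights, emissive screen and construction-built indicators that count down remaining time, then stop the cables and restore the configured on/off look.
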(event `self.Health.OnDamage`
  (params (DamageContext :type "DamageContext Structure (by ref)"))
  (bind _actor_light_areaflicker (`self.Actor Light AreaFlicker`))
  (bind _health (`self.Health`))
  (bind _returnvalue (`self.GetComponentByClass` _actor_light_areaflicker "/Game/Design/GPE/Interactables/BP_AreaControllerFlickeringComponent.BP_AreaControllerFlickeringComponent_C"))
  ;[0 0 0 1 25] Take Damage
  (if (`|EnumEquality` DamageContext_DamageType "Shock")
    (`|ExecutionSequence`
      (:`then_0`
        (bind _cables (`self.Cables`)
          (:`then`
            (`/Game/Art/VFX/GPE/Lightnings/BP_CableToActivate.ActivateLightning` _cables))
          (:`else`
            _))
        (`/Engine/EditorBlueprintResources/StandardMacros.IsValid` _actor_light_areaflicker
          (:`Is Valid`
            (if (> (/ (`HealthComponent.CurrentHealth` _health) (`HealthComponent.MaxHealth` _health)) 0.5)
              (`/Game/Design/GPE/Interactables/BP_AreaControllerFlickeringComponent.Take Damage Actualisation Area` _returnvalue "/Game/Design/_GameManagement/Light/C_Flickering_Sequence_SwitchOn.C_Flickering_Sequence_SwitchOn")
              (else
                (`/Game/Design/GPE/Interactables/BP_AreaControllerFlickeringComponent.Take Damage Actualisation Area` _returnvalue "/Game/Design/_GameManagement/Light/C_Flickering_Sequence_SwitchOn_long.C_Flickering_Sequence_SwitchOn_long"))))))
      (:`then_1`
        (`/Engine/EditorBlueprintResources/StandardMacros.DoOnce` false
          (:`Completed`
            (`/EventDispatcherHub/FunctionLibrary/BPL_EventDispatcherHub.Call Single Gameplay Event` (`self.Tag to Call`) self)))))))

(event `self.ReceiveTick`
  (params (DeltaSeconds :type "Float (single-precision)"))
  ;[0 0 0 1 25] Take Damage
  (`HealthComponent.Heal` (`self.Health`) 5))

(event `ReFresh State`
  ;[1 0 0 0.999 50] STATE BEHAVIOR
  (if (`self.Should OFF`) :!label _label
    (`self.Set All Parameter FeedBack` (`|GetArrayItem` (`self.Materials`)) (`self.Light OFF Color`) (`self.New Light Function Material`))
    (`self.UpdateLightIndicators` (struct) true)
    (else
      (`self.Set All Parameter FeedBack` (`self.Material ON`) (`self.Light ON Color`))
      (`self.UpdateLightIndicators` (struct) true true))))

(event `self.ReceiveBeginPlay`
  (bind _tag_receive (`self.Tag Receive`))
  (bind _saveload (`self.SaveLoad`))
  (`parent.ReceiveBeginPlay`)
  (`|ExecutionSequence`
    (:`then_0`
      (if (`BlueprintGameplayTagLibrary.IsGameplayTagValid` _tag_receive)
        (`/EventDispatcherHub/FunctionLibrary/BPL_EventDispatcherHub.Bind to Single Gameplay Event` _tag_receive self))
      (set `self.MyTriggerComponents` (`self.K2_GetComponentsByClass` "/Game/Design/EnvironmentEvents/Components/BP_TriggerEventReceiver_Component.BP_TriggerEventReceiver_Component_C"))
      (if (`self.ShouldStartOn`)
        (bind _returnvalue (`GameplayStatics.GetActorOfClass` "/Game/Art/VFX/GPE/Lightnings/BP_CableToActivate.BP_CableToActivate_C"))
        (set `self.Cables` _returnvalue)))
    (:`then_1`
      ;[1 1 1 0.33] Force Load if the Actor is initialized to late on the level streaming
      (if (not (`SaveLoadComponent.bIsDataLoaded` _saveload))
        (`SaveLoadComponent.Load` _saveload)))
    (:`then_2`
      ;[1 1 1 0.33 42] STORAGE DATA
      (`PrimitiveComponent.CreateDynamicMaterialInstance` (`self.FeedBackWidget`) 0 null "None")
      (set `self.Original Light Intensity` (`LightComponentBase.Intensity` (`self.PointLight`)))
      (`KismetArrayLibrary.Array_Add` (`self.Materials`) (`PrimitiveComponent.GetMaterial` (`self.FeedBackWidget`) 2))
      (set `self.New Light Function Material` (`LightComponent.LightFunctionMaterial` (`self.Light`)))
      (goto _label))))

(event `self.SaveLoad.OnLoadActor`
  (bind _value (`StructUtilsFunctionLibrary.GetInstancedStructValue` (`SaveLoadComponent.SavedData` (`self.SaveLoad`)))
    (:`Valid`
      (if (`.bIsConsummed` (break `InteractableSavedData` _value))
        _))))

(fn `CanCallTakeDamage`
  (params (DamageContext :type "DamageContext Structure (by ref)"))
  (returns (ReturnValue :type Boolean))
  (return true))

(fn `IsShownAsDamageableToPlayer`
  (params (DamageType :type "EDamageType Enum" :default "Generic"))
  (returns (ReturnValue :type Boolean))
  (return (`|EnumEquality` DamageType "Shock")))

(fn `OnFlickLightStart`
  (params (LightData :type "LightData Structure (by ref)"))
  (setmembers `LightData` :`StructRef` LightData :`OriginalLightIntensity` (`self.Original Light Intensity`))
  (`PrimitiveComponent.SetMaterial` (`self.FeedBackWidget`) 2 (`self.Material ON`))
  (return))

(fn `OnFlickLightStop`
  (params (LightData :type "LightData Structure (by ref)"))
  (`self.UpdateLightIndicators` LightData)
  (bind _cables (`self.Cables`)
    (:`then`
      (`/Game/Art/VFX/GPE/Lightnings/BP_CableToActivate.DeactivateLightning` _cables))
    (:`else`
      _))
  (if (`self.Should OFF`)
    (`self.Set All Parameter FeedBack` (`|GetArrayItem` (`self.Materials`)) (`self.Light OFF Color`) (`self.New Light Function Material`))
    (else
      (`self.Set All Parameter FeedBack` (`self.Material ON`) (`self.Light ON Color`))))
  (return))

(fn `OnFlickLightTick`
  (params (DeltaTime :type "Float (single-precision)") (LightData :type "LightData Structure (by ref)"))
  (return))

(fn `OnFlickLightUpdate`
  (params (LightData :type "LightData Structure (by ref)") (IntensityScale :type "Float (single-precision)"))
  (bind _returnvalue (* (`self.Original Light Intensity`) IntensityScale))
  (`LightComponent.SetIntensity` (`self.Light`) _returnvalue)
  (`LightComponent.SetIntensity` (`self.PointLight`) _returnvalue)
  (`self.Set All Parameter FeedBack` null (`self.Light ON Color`))
  (bind _returnvalue_2 (`PrimitiveComponent.CreateDynamicMaterialInstance` (`self.FeedBackWidget`) 2 "/Game/Art/LevelPrototyping/Lights/Emissives/M_NeonGreen.M_NeonGreen" "None"))
  (`MaterialInstanceDynamic.SetScalarParameterValue` _returnvalue_2 "Emissive" _returnvalue)
  (`self.UpdateLightIndicators` LightData)
  (return))

(fn `ReceiveEvent`
  (params (CalledTag :type "GameplayTag Structure") (CallingObject :type "Object Object Reference (by ref)"))
  (returns (Return :type Boolean))
  (`|SwitchGameplayTag` CalledTag
    (:`Event.Room.After1stRift.1stBackTrack`
      (return false))))

(fn `RetrieveFlickableLights`
  (returns (ReturnValue :type "Array of LightComponent Object Reference"))
  (return (`|MakeArray` (`self.Light`) (`self.PointLight`) :!type "LightComponent Object Reference")))

(fn `SaveConsumeInteraction`
  (bind _saveddata (`SaveLoadComponent.SavedData` (`self.SaveLoad`)))
  (bind _value (`StructUtilsFunctionLibrary.GetInstancedStructValue` _saveddata)
    (:`Valid`
      (bind _structout (setmembers `InteractableSavedData` :`StructRef` _value :`bIsConsummed` true))
      (`StructUtilsFunctionLibrary.SetInstancedStructValue` _saveddata _structout))))

(fn `Set All Parameter FeedBack`
  (params (Material :type "MaterialInterface Object Reference") (NewLightColor :type "LinearColor Structure") (NewLightFunctionMaterial :type "MaterialInterface Object Reference"))
  (`PrimitiveComponent.SetMaterial` (`self.FeedBackWidget`) 2 Material)
  (`LightComponent.SetLightColor` (`self.Light`) NewLightColor true)
  (`LightComponent.SetLightColor` (`self.PointLight`) NewLightColor true)
  (`LightComponent.SetLightFunctionMaterial` (`self.PointLight`) NewLightFunctionMaterial))

(fn `TakeDamage`
  (params (DamageContext :type "DamageContext Structure (by ref)"))
  (returns (ReturnValue :type Boolean))
  (switch `EDamageType` DamageContext_DamageType
    (:`Generic`
      _)
    (:`Bullet`
      _)
    (:`Melee`
      _)
    (:`Shock`
      (return true))
    (:`Explosion`
      _))
  (return false))

(fn `UpdateLightIndicators`
  (params (LightData :type "LightData Structure (by ref)") (bIsForced :type Boolean) (bForcedValue :type Boolean))
  (bind (_originallightfunction _currentlightfunction _originallightintensity _originalemissivepower _lightcomponent _startworldtime _timeduration) (break `LightData` LightData))
  (for (_array_element _array_index) (`self.LightIndicators`)
    (if (`local.bIsForced`)
      (`PrimitiveComponent.SetMaterial` _array_element 0 (select `bool` (`local.bForcedValue`) :`false` "/Game/Art/0_Materials/Material_Instance/Flat/MI_FlatColor_Black.MI_FlatColor_Black" :`true` "/Game/Art/LevelPrototyping/Lights/Emissives/M_FlickeringNeonBright.M_FlickeringNeonBright" :!type "MaterialInterface Object Reference"))
      (else
        (`PrimitiveComponent.SetMaterial` _array_element 0 (select `bool` (> (- 1.0 (/ (- (`KismetSystemLibrary.GetGameTimeInSeconds`) _startworldtime) _timeduration)) (/ _array_index (`KismetArrayLibrary.Array_Length` (`self.LightIndicators`)))) :`false` "/Game/Art/0_Materials/Material_Instance/Flat/MI_FlatColor_Black.MI_FlatColor_Black" :`true` "/Game/Art/LevelPrototyping/Lights/Emissives/M_FlickeringNeonBright.M_FlickeringNeonBright" :!type "MaterialInterface Object Reference"))))))

(fn `UserConstructionScript`
  (locals (EndLocation :type "Vector Structure" :default (0.0 20.0 0.0)) (NumberOfIndicators :type Integer :default 8))
  (bind _lightindicator0 (`self.LightIndicator0`))
  (bind _returnvalue (- (`local.NumberOfIndicators`) 1))
  (set `local.EndLocation` (`KismetMathLibrary.NegateVector` (`SceneComponent.RelativeLocation` (`self.LightIndicator0`))))
  (`KismetArrayLibrary.Array_Add` (`self.LightIndicators`) (`self.LightIndicator0`))
  (for _index (range (+ _returnvalue 1))
    (bind _returnvalue_2 (`AddComponent|NODE_AddStaticMeshComponent-0` :`RelativeTransform` (`KismetMathLibrary.MakeTransform` (`KismetMathLibrary.VLerp` (`SceneComponent.RelativeLocation` (`self.LightIndicator0`)) (`local.EndLocation`) (/ _index _returnvalue)) (struct) (`SceneComponent.RelativeScale3D` _lightindicator0))))
    (`StaticMeshComponent.SetStaticMesh` _returnvalue_2 (`StaticMeshComponent.StaticMesh` _lightindicator0))
    (`PrimitiveComponent.SetMaterial` _returnvalue_2 0 (`PrimitiveComponent.GetMaterial` (`self.LightIndicator0`) 0))
    (`SceneComponent.K2_AttachToComponent` _returnvalue_2 (`self.LightIndicatorPivot`) "None" "KeepRelative" "KeepRelative" "KeepRelative" true)
    (`KismetArrayLibrary.Array_Add` (`self.LightIndicators`) _returnvalue_2)))