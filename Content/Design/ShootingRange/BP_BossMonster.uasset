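; Shooting range boss monster that spins at a set rotation speed and advances through stages as its weak points are destroyed.
; On BeginPlay it binds each weak point's Health OnDeath event to UpdateCurrentStage, while Tick yaws the capsule.
; Each death increments a never-reset OrgansDown count, compared with the current stage's threshold in the StagesInfo map.
; Stage changes only increment CurrentStage and print debug text.
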(event `self.ReceiveBeginPlay`
  ;[0.4802 0 0.01596 0.33] BEGINPLAY
  (`parent.ReceiveBeginPlay`)
  ;;[1 1 1 0.33] Bind WeakPoint's LifeComponent Event OnDeath
  (for _array_element (`self.WeakPoints`)
    (add `HealthComponent.OnDeath` (`/Game/Design/EyeVisionSystem/BP_WeakPoints.Health` _array_element) (delegate `OnWeakPointDown`))))

(event `OnWeakPointDown`
  (params (DamageContext :type "DamageContext Structure (by ref)"))
  ;[0.4802 0 0.01596 0.33] BEGINPLAY
  (`self.UpdateCurrentStage`))

(event `self.ReceiveTick`
  (params (DeltaSeconds :type "Float (single-precision)"))
  ;[1 1 1 0.33] ROTATOR
  (`SceneComponent.K2_AddWorldRotation` (`self.CapsuleComponent`) (`KismetMathLibrary.MakeRotator` 0.0 0.0 (`self.RotationSpeed`)) false false))

(fn `UpdateCurrentStage`
  (bind _result (`/Engine/EditorBlueprintResources/StandardMacros.IncrementInt` (`self.OrgansDown`))
    (:`  `
      (if (>= _result (`BlueprintMapLibrary.Map_Find` (`self.StagesInfo`) (`self.CurrentStage`)))
        (`KismetSystemLibrary.PrintString` "Next Boss Stage !" true true (struct :`R` 1.0 :`B` 0.016606 :`A` 1.0))
        (`/Engine/EditorBlueprintResources/StandardMacros.IncrementInt` (`self.CurrentStage`))
        (else
          (`KismetSystemLibrary.PrintString` "Organs HIT !" true true (struct :`G` 0.265401 :`B` 1.0 :`A` 1.0)))))))

(fn `UserConstructionScript`)