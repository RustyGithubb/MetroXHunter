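; Cheat function that clears the default ammo in the player's inventory.
; One tick after init, it caches the BP_InventoryComponent of the pawn controlled by the cheat manager's player controller.
; When the cheat fires, it calls ClearDefaultAmmo on that component if the cached reference is valid.
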(event `self.OnInit`
  (`KismetSystemLibrary.DelayUntilNextTick`)
  (`self.RegisterInventoryComponent`))

(event `self.OnCheat`
  (bind _playerinventorycomponent (`self.PlayerInventoryComponent`)
    (:`then`
      (`/Game/0_Design/GameManagement_/BP_InventoryComponent.ClearDefaultAmmo` _playerinventorycomponent))
    (:`else`)))

(fn `RegisterInventoryComponent`
  (bind _returnvalue (`Controller.K2_GetPawn` (`CheatManager.GetPlayerController` (`self.CheatManager`))))
  (`/Engine/EditorBlueprintResources/StandardMacros.IsValid` _returnvalue
    (:`Is Valid`
      (set `self.PlayerInventoryComponent` (`Actor.GetComponentByClass` _returnvalue "/Game/0_Design/GameManagement_/BP_InventoryComponent.BP_InventoryComponent_C")))))