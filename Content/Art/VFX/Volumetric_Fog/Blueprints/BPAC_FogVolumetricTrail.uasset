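; Actor component that gives its owner a Niagara trail in volumetric fog and feeds its position to the fog.
; Shortly after BeginPlay, a valid Instigator selects the forward-offset character trail; otherwise it uses the object trail with IgnoreZ set.
; The attached system receives TrailSize.
; Every tick, owner location and Radius are packed into the shared PlayerPos parameter of MPC_FogVolumetrics, so multiple instances overwrite one another.
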(event `self.ReceiveBeginPlay`
  (`KismetSystemLibrary.Delay` 0.1)
  (`/Engine/EditorBlueprintResources/StandardMacros.IsValid` (`Actor.Instigator` (`self.GetOwner`))
    (:`Is Valid`
      (set `self.IsCharacter` true))
    (:`Is Not Valid`
      (set `self.IsCharacter` false)))
  (bind _nsreference (`/Game/Art/VFX/Volumetric_Fog/Blueprints/BPFL_FogVolumetric.FogVolumetricSystemAttached` (select `bool` (`self.IsCharacter`) :`false` "/Game/Art/VFX/Volumetric_Fog/VFX/NS_FogObjectsTrail.NS_FogObjectsTrail" :`true` "/Game/Art/VFX/Volumetric_Fog/VFX/NS_FogCharacterTrail.NS_FogCharacterTrail" :!type "NiagaraSystem Object Reference") (`Actor.RootComponent` (`self.GetOwner`)) (`KismetMathLibrary.SelectVector` (30.0 0.0 0.0) (0.0 0.0 0.0) (`self.IsCharacter`))))
  (bind _output_get (set `self.TrailReference` _nsreference))
  (`/Engine/EditorBlueprintResources/StandardMacros.IsValid` _output_get
    (:`Is Valid`
      (`NiagaraComponent.SetVariableFloat` _output_get "TrailSize" (`self.TrailSize`))
      (if (not (`self.IsCharacter`))
        (`NiagaraComponent.SetVariableBool` _output_get "IgnoreZ" true)))))

(event `self.ReceiveTick`
  (params (DeltaSeconds :type "Float (single-precision)"))
  (bind (_returnvalue_x _returnvalue_y _returnvalue_z) (`KismetMathLibrary.BreakVector` (`Actor.K2_GetActorLocation` (`self.GetOwner`))))
  (`KismetMaterialLibrary.SetVectorParameterValue` "/Game/Art/VFX/Volumetric_Fog/Material/MPC_FogVolumetrics.MPC_FogVolumetrics" "PlayerPos" (`KismetMathLibrary.MakeColor` _returnvalue_x _returnvalue_y _returnvalue_z (`self.Radius`))))