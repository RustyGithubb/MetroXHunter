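; Trigger receiver component that plays a configured sound when its component-specific play event fires.
; Radio calls play a start cue plus the sound in 2D, but the end cue after the delay is disconnected.
; Otherwise it plays a stored 2D sound or one at an actor or owner-offset location, previewed by a debug box.
; Gameplay-tag binding, stopping and calling are unwired, and ReceiveEvent just returns false.
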(event `Sound end`
  (params (Sound :type "SoundBase Object Reference") (VolumeMultiplier :type "Float (single-precision)") (PitchMultiplier :type "Float (single-precision)") (StartTime :type "Float (single-precision)"))
  (`KismetSystemLibrary.Delay` (`SoundBase.Duration` Sound)))

(fn `DisplaySoundLocation`
  (`KismetSystemLibrary.FlushPersistentDebugLines`)
  (`KismetSystemLibrary.DrawDebugBox` (+ (`Actor.K2_GetActorLocation` (`self.GetOwner`)) (`self.RelativePlayLocation`)) (5.0 5.0 5.0) (struct :`R` 1.0 :`B` 1.0 :`A` 1.0) (struct) 10.0 5.0))

(fn `OnPlayComponentSpecificEvent`
  (params (FromBoxEnter :type Boolean) (TriggerBox :type "Actor Object Reference"))
  (bind _volume_multiplier (`self.Volume Multiplier`))
  (bind _pitch_multiplier (`self.Pitch Multiplier`))
  (bind _start_time (`self.Start Time`))
  ;[1 0.6524 0.3523 0.33 30] Archive
  (bind _soundstoplay (`self.SoundsToPlay`)
    (:`then`
      (if (`self.Radio call`)
        (`GameplayStatics.PlaySound2D` "/Game/Sounds/Audio/SFX/Radio/SW_Radio_Start.SW_Radio_Start" 1.0 1.0 0.0 null null)
        (`GameplayStatics.PlaySound2D` _soundstoplay _volume_multiplier _pitch_multiplier _start_time null (`self.GetOwner`))
        (`self.Sound end` _soundstoplay _volume_multiplier _pitch_multiplier _start_time)
        (elif (`self.PlaySound2D`)
          (bind _returnvalue (`GameplayStatics.SpawnSound2D` _soundstoplay (`self.Volume Multiplier`) (`self.Pitch Multiplier`) (`self.Start Time`) null))
          (set `self.CurrentSound` _returnvalue)
          (elif (`self.is actor location`)
            (`GameplayStatics.PlaySoundAtLocation` _soundstoplay (`Actor.K2_GetActorLocation` (`self.Actor`)) (struct) (`self.Volume Multiplier`) (`self.Pitch Multiplier`) (`self.Start Time`) (`self.Attenuation Settings`) null (`self.GetOwner`) null)
            (else
              (`GameplayStatics.PlaySoundAtLocation` _soundstoplay (+ (`Actor.K2_GetActorLocation` (`self.GetOwner`)) (`self.RelativePlayLocation`)) (struct) (`self.Volume Multiplier`) (`self.Pitch Multiplier`) (`self.Start Time`) (`self.Attenuation Settings`) null (`self.GetOwner`) null))))))
    (:`else`)))

(fn `ReceiveEvent`
  (params (CalledTag :type "GameplayTag Structure") (CallingObject :type "Object Object Reference (by ref)"))
  (returns (Return :type Boolean))
  (return false))