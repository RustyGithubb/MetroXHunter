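; Temporary player gun that fires hitscan shots, spending ammo through the player's ReloadComponent, which also gates CanFire.
; A camera trace, randomized by movement imprecision, sets the target for a muzzle sphere trace.
; Its first two hits drive HealthComponent damage or surface-based water and bullet-impact effects.
; Shots also trigger camera shake, sound, AI noise and gameplay events, while Tick draws a spread-free debug-line laser when aiming.
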(event `self.ReceiveBeginPlay`
  ;[1 1 1 0.33] Comment
  (bind _asbp_main_chara (cast `/Game/Design/_GameManagement/BP_MainChara` (`GameplayStatics.GetPlayerCharacter` 0)))
  (bind _output_get (set `self.PlayerCharacter` _asbp_main_chara))
  (set `self.ReloadSystem` (`self.GetComponentByClass` _output_get "/Script/MetroXHunter.ReloadComponent")))

(event `Trigger Shoot`
  (params (ImpactDirection :type "Vector Structure"))
  (bind (_returnvalue_location _returnvalue_rotation) (`KismetMathLibrary.BreakTransform` (`SceneComponent.K2_GetComponentToWorld` (`self.ShootPoint`))))
  (`ReloadComponent.DecrementAmmo` (`self.ReloadSystem`))
  ;[0 0 0 0.33 55] CAMERA SEQUENCER SHAKE
  (`CameraShakeSourceComponent.Start` (`self.CameraShakeSource`))
  ;[1 0 0 0.33 55] DATA DEBUG
  (`/EventDispatcherHub/FunctionLibrary/BPL_EventDispatcherHub.Call Single Gameplay Event` (struct :`TagName` "Event.mainCharacter.Shoot") self)
  (`self.MakeNoise` 1.0 (`self.PlayerCharacter`)) ; Alert AIs that a noise occured
  ;[1 1 1 0.33] CHECK IF HEALTH COMPONENT
  (`|ExecutionSequence`
    (:`then_0`
      (bind _impactpoint (`self.CalculateWorldLocation` true))
      (bind (_outhits _returnvalue) (`KismetSystemLibrary.SphereTraceMulti` :`Start` (`SceneComponent.K2_GetComponentLocation` (`self.ShootPoint`)) :`End` _impactpoint :`Radius` 5.0 :`TraceChannel` "TraceTypeQuery3" :`TraceColor` (struct :`R` 1.0 :`B` 0.75 :`A` 1.0) :`TraceHitColor` (struct :`G` 0.88723 :`B` 1.0 :`A` 1.0)))
      (if _returnvalue
        (set `self.bAlreadyHit` false)
        (for (_array_element _array_index) _outhits
          (if (< _array_index 2)
            (bind (_bblockinghit _binitialoverlap _time _distance _location _impactpoint_2 _normal _impactnormal _physmat _hitactor) (`GameplayStatics.BreakHitResult` _array_element))
            (set `self.Impact Point` _impactpoint_2)
            (bind _returnvalue_2 (`self.GetComponentByClass` _hitactor "/Script/MetroXHunter.HealthComponent"))
            ;;[1 1 1 0.33] Damage Health Component on Hit Actor (if has one)
            (`/Engine/EditorBlueprintResources/StandardMacros.IsValid` _returnvalue_2
              (:`Is Valid`
                (if (not (`self.bAlreadyHit`))
                  (set `self.bAlreadyHit` true)
                  (`HealthComponent.TakeDamage` _returnvalue_2 (make `DamageContext` (`self.GunDamageAmount`) "Bullet" (`self.PlayerCharacter`) self _array_element))
                  (`/EventDispatcherHub/FunctionLibrary/BPL_EventDispatcherHub.Call Single Gameplay Event` (struct :`TagName` "Event.mainCharacter.ShotHit") self)
                  ;[1 1 1 0.33] Spawn Muzzle Flash + Smoke
                  (`NiagaraFunctionLibrary.SpawnSystemAtLocation` "/Game/Art/VFX/NS_Muzzle_Flash_Multiple.NS_Muzzle_Flash_Multiple" _returnvalue_location _returnvalue_rotation)))
              (:`Is Not Valid`
                (set `self.bAlreadyHit` false)
                ;[1 1 1 0.33] Spawn Impulse effect on water
                (if (`|EnumEquality` (`PhysicalMaterial.SurfaceType` _physmat) "SurfaceType1")
                  (`|SpawnActorFromClass` "/Game/Art/VFX/GPE/Water/BP_Fluid_Impulse_Repeating_Test.BP_Fluid_Impulse_Repeating_Test_C" (`KismetMathLibrary.Conv_VectorToTransform` _impactpoint_2) "AlwaysSpawn" "MultiplyWithRoot" null null)
                  ;[1 1 1 0.33] Spawn Splash Effect
                  (`NiagaraFunctionLibrary.SpawnSystemAtLocation` "/Game/Art/VFX/NS_Water_Splash.NS_Water_Splash" _impactpoint_2)
                  (else
                    ;[1 1 1 0.33] Spawn Bullet Decal
                    (`|SpawnActorFromClass` "/Game/Art/VFX/GPE/Gun/BP_Bullet_Decals.BP_Bullet_Decals_C" (`KismetMathLibrary.MakeTransform` _impactpoint_2 (`KismetMathLibrary.Conv_VectorToRotator` _normal) (`self.BulletHoleSize`)) "AlwaysSpawn" "MultiplyWithRoot" null null)
                    ;[1 1 1 0.33] Spawn FX Structures Impact and fix the facing directions
                    (`NiagaraFunctionLibrary.SpawnSystemAtLocation` "/Game/Art/VFX/NS_Impact_Struct.NS_Impact_Struct" _impactpoint_2 (`KismetMathLibrary.FindLookAtRotation` _impactpoint_2 (`self.K2_GetActorLocation` (`self.PlayerCharacter`))))
                    (`NiagaraFunctionLibrary.SpawnSystemAtLocation` "/Game/Art/VFX/NS_Muzzle_Flash_Multiple.NS_Muzzle_Flash_Multiple" _returnvalue_location _returnvalue_rotation)))))))))
    (:`then_1`
      (`GameplayStatics.PlaySoundAtLocation` "/Game/Sounds/Placeholders/Character/Gun/SC_GunShot.SC_GunShot" (`SceneComponent.K2_GetComponentLocation` (`self.ShootPoint`)) (struct) 1.0 1.0 0.0 null null null null))))

(event `self.ReceiveTick`
  (params (DeltaSeconds :type "Float (single-precision)"))
  ;[1 0.05208 0.05208 0.458] Laser Pointer to tell where we're actually gonna shoot
  (if (`/Game/Design/_GameManagement/BP_MainChara.bIsAiming` (`self.PlayerCharacter`))
    (bind _impactpoint (`self.CalculateWorldLocation` false))
    (bind (_outhits _returnvalue) (`KismetSystemLibrary.SphereTraceMulti` :`Start` (`SceneComponent.K2_GetComponentLocation` (`self.ShootPoint`)) :`End` _impactpoint :`Radius` 5.0 :`TraceChannel` "TraceTypeQuery3" :`TraceColor` (struct :`R` 1.0 :`B` 0.75 :`A` 1.0) :`TraceHitColor` (struct :`G` 0.88723 :`B` 1.0 :`A` 1.0)))
    (if _returnvalue
      (`KismetSystemLibrary.DrawDebugLine` (`SceneComponent.K2_GetComponentLocation` (`self.ShootPoint`)) (`.ImpactPoint` (`GameplayStatics.BreakHitResult` (`|GetArrayItem` _outhits))) (struct :`R` 1.0 :`A` 1.0) 0.025 0.7))))

(fn `CalculateWorldLocation`
  (params (UseMovementImprecision :type Boolean :default true))
  (returns (ImpactPoint :type "Vector Structure"))
  (bind _cinecamera (`/Game/Design/_GameManagement/BP_MainChara.CineCamera` (`self.PlayerCharacter`)))
  (bind _returnvalue (`SceneComponent.K2_GetComponentLocation` _cinecamera))
  (bind _returnvalue_2 (`SceneComponent.GetForwardVector` _cinecamera))
  (bind _returnvalue_3 (* (`/Game/Design/_GameManagement/BP_MainChara.ShootingImprecisionValue` (`self.PlayerCharacter`)) 1000.0))
  (bind _returnvalue_4 (* _returnvalue_3 -1.0))
  (bind _outhit (`KismetSystemLibrary.LineTraceSingle` (+ _returnvalue (* _returnvalue_2 110)) (+ (+ _returnvalue (* _returnvalue_2 30000)) (`KismetMathLibrary.SelectVector` (`KismetMathLibrary.MakeVector` (`KismetMathLibrary.RandomFloatInRange` _returnvalue_4 _returnvalue_3) (`KismetMathLibrary.RandomFloatInRange` _returnvalue_4 _returnvalue_3) (`KismetMathLibrary.RandomFloatInRange` _returnvalue_4 _returnvalue_3)) (0.0 0.0 0.0) UseMovementImprecision)) "TraceTypeQuery3"))
  (return (`.ImpactPoint` (`GameplayStatics.BreakHitResult` _outhit))))

(fn `CanFire`
  (returns (CanFire :type Boolean))
  ;[1 1 1 0.33] Check Gun is not Locked from Reload System
  (if (not (`ReloadComponent.IsReloading` (`self.ReloadSystem`)))
    ;[1 1 1 0.33] Check Magazine
    (if (not (`ReloadComponent.IsGunEmpty` (`self.ReloadSystem`)))
      (return true)
      (else
        (`KismetSystemLibrary.PrintString` "NeedReload")))
    (else
      (`KismetSystemLibrary.PrintString` "Gun: Fire is locked from ReloadSystem!" true true (struct :`R` 1.0 :`A` 1.0))))
  (return false))

(fn `UserConstructionScript`)