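; Cheat function that refills the player's ammo to maximum.
; One tick after init, it caches the inventory and QTE reload components from the controlled pawn.
; On activation, it fills all ammo, then sets the reload state and fires its update call so the backpack ammo widget refreshes without showing the QTE bar.
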(event `self.OnInit`
  (`KismetSystemLibrary.DelayUntilNextTick`)
  (`self.RegisterInventoryComponent`))

(event `self.OnCheat`
  (bind _reloadcomponent (`self.ReloadComponent`))
  (bind _playerinventory (`self.PlayerInventory`)
    (:`then`
      (`InventoryComponent.FullyFillAmmo` _playerinventory)
      ;[1 1 1 0.33] Call OnReloadStateUpdated to update the Widget showing the backpack ammo, But also set the State on NormalFinished otherwise it'll show the QTE bar
      (`/Game/Design/ReloadSystem/BP_ReloadSystemComponent_QTE.UpdateCurrentReloadState` _reloadcomponent "NewEnumerator1")
      (`/Game/Design/ReloadSystem/BP_ReloadSystemComponent_QTE.OnReloadStateUpdated` _reloadcomponent))
    (:`else`)))

(fn `RegisterInventoryComponent`
  (bind _returnvalue (`Controller.K2_GetPawn` (`CheatManager.GetPlayerController` (`self.CheatManager`))))
  (`/Engine/EditorBlueprintResources/StandardMacros.IsValid` _returnvalue
    (:`Is Valid`
      (set `self.PlayerInventory` (`Actor.GetComponentByClass` _returnvalue "/Script/MetroXHunter.InventoryComponent"))
      (set `self.ReloadComponent` (`Actor.GetComponentByClass` _returnvalue "/Game/Design/ReloadSystem/BP_ReloadSystemComponent_QTE.BP_ReloadSystemComponent_QTE_C")))))