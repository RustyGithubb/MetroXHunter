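; Debug camera controller that lets the cheat menu keys exit the debug camera.
; On BeginPlay it caches the keys bound to IA_CheatMenu in IMC_Default, then checks every key press against them to call DisableDebugCamera on the CheatManager.
; While active, it prints an on-screen hint each tick listing those keys by display name.
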(event `Key|AnyKey` :consume false
  (params (Key :type "Key Structure"))
  (:`Pressed`
    (for _array_element (`self.CheatActionKeys`)
      (if (== _array_element Key)
        (`CheatManager.DisableDebugCamera` (`self.CheatManager`))
        (break)))))

(event `self.ReceiveBeginPlay`
  (bind _keys (`/Game/Design/Libraries/BPL_InputPlus.FindActionKeys` "/Game/Design/_GameManagement/Input/Player/IMC_Default.IMC_Default" "/Game/Design/_GameManagement/Input/IA_CheatMenu.IA_CheatMenu"))
  (set `self.CheatActionKeys` _keys))

(event `self.ReceiveTick`
  (params (DeltaSeconds :type "Float (single-precision)"))
  (if (`self.IsActivated`)
    (`KismetSystemLibrary.PrintText` (`|FormatText` "DebugCamera: Press {ConcatenatedKeys} to disable the debug camera" (`self.ConcatenateCheatKeys`)) true true (struct :`R` 1.0 :`G` 0.083333 :`A` 1.0) DeltaSeconds "DisableDebugCamera")))

(event `self.ReceiveOnActivate`
  (params (OriginalPC :type "PlayerController Object Reference"))
  (set `self.IsActivated` true))

(event `self.ReceiveOnDeactivate`
  (params (RestoredPC :type "PlayerController Object Reference"))
  (set `self.IsActivated` false))

(fn `ConcatenateCheatKeys`
  (returns (String :type String))
  (locals (KeyNames :type "Array of String"))
  (for _array_element (`self.CheatActionKeys`)
    (`KismetArrayLibrary.Array_Add` (`local.KeyNames`) (`KismetTextLibrary.Conv_TextToString` (`|FormatText` "'{Key}'" (`KismetInputLibrary.Key_GetDisplayName` _array_element)))))
  (return (`KismetStringLibrary.JoinStringArray` (`local.KeyNames`) ", ")))

(fn `UserConstructionScript`)