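; BP_BigMonster is a rotating shooting-range monster that exposes weak points while targeted.
; Tick spins the root at a set rotation speed.
; OnTargeted swaps body-part materials to an alpha brown and enables each weak point with the player camera, then restores flat brown and disables them when untargeted.
; LeftLeg3 is missing from the restore list, and the EnableWeakPoints function is empty.
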(event `self.ReceiveTick`
  (params (DeltaSeconds :type "Float (single-precision)"))
  ;[1 1 1 0.33] ROTATOR
  (`SceneComponent.K2_AddWorldRotation` (`self.DefaultSceneRoot`) (`KismetMathLibrary.MakeRotator` 0.0 0.0 (`self.RotationSpeed_0`)) false false))

(event `self.ReceiveBeginPlay`
  (`parent.ReceiveBeginPlay`))

(event `self.OnTargeted`
  (params (IsTargeted :type Boolean) (PlayerCamera :type "CineCameraComponent Object Reference"))
  (bind _head (`self.Head`))
  (if IsTargeted
    (`PrimitiveComponent.SetMaterial` _head 0 "/Game/9_ShootingRange/Materials/MI_FlatColor_Alpha_Brown.MI_FlatColor_Alpha_Brown")
    (`PrimitiveComponent.SetMaterial` (`self.Mouth`) 0 "/Game/9_ShootingRange/Materials/MI_FlatColor_Alpha_Brown.MI_FlatColor_Alpha_Brown")
    (`PrimitiveComponent.SetMaterial` (`self.Body`) 0 "/Game/9_ShootingRange/Materials/MI_FlatColor_Alpha_Brown.MI_FlatColor_Alpha_Brown")
    (`PrimitiveComponent.SetMaterial` (`self.LeftLeg3`) 0 "/Game/9_ShootingRange/Materials/MI_FlatColor_Alpha_Brown.MI_FlatColor_Alpha_Brown")
    (`PrimitiveComponent.SetMaterial` (`self.LeftLeg2`) 0 "/Game/9_ShootingRange/Materials/MI_FlatColor_Alpha_Brown.MI_FlatColor_Alpha_Brown")
    (`PrimitiveComponent.SetMaterial` (`self.LeftLeg`) 0 "/Game/9_ShootingRange/Materials/MI_FlatColor_Alpha_Brown.MI_FlatColor_Alpha_Brown")
    (`PrimitiveComponent.SetMaterial` (`self.RightLeg`) 0 "/Game/9_ShootingRange/Materials/MI_FlatColor_Alpha_Brown.MI_FlatColor_Alpha_Brown")
    (`PrimitiveComponent.SetMaterial` (`self.RightLeg4`) 0 "/Game/9_ShootingRange/Materials/MI_FlatColor_Alpha_Brown.MI_FlatColor_Alpha_Brown")
    (`PrimitiveComponent.SetMaterial` (`self.RightLeg3`) 0 "/Game/9_ShootingRange/Materials/MI_FlatColor_Alpha_Brown.MI_FlatColor_Alpha_Brown")
    (`PrimitiveComponent.SetMaterial` (`self.RightLeg2`) 0 "/Game/9_ShootingRange/Materials/MI_FlatColor_Alpha_Brown.MI_FlatColor_Alpha_Brown")
    (`PrimitiveComponent.SetMaterial` (`self.LeftLeg1`) 0 "/Game/9_ShootingRange/Materials/MI_FlatColor_Alpha_Brown.MI_FlatColor_Alpha_Brown")
    (for _array_element (`self.WeakPoints`)
      (`/Game/0_Design/EyeVisionSystem/BP_WeakPoints.Enable` _array_element PlayerCamera))
    (else
      (`PrimitiveComponent.SetMaterial` _head 0 "/Game/9_ShootingRange/Materials/MI_FlatColor_Brown.MI_FlatColor_Brown")
      (`PrimitiveComponent.SetMaterial` (`self.Mouth`) 0 "/Game/9_ShootingRange/Materials/MI_FlatColor_Brown.MI_FlatColor_Brown")
      (`PrimitiveComponent.SetMaterial` (`self.Body`) 0 "/Game/9_ShootingRange/Materials/MI_FlatColor_Brown.MI_FlatColor_Brown")
      (`PrimitiveComponent.SetMaterial` (`self.LeftLeg2`) 0 "/Game/9_ShootingRange/Materials/MI_FlatColor_Brown.MI_FlatColor_Brown")
      (`PrimitiveComponent.SetMaterial` (`self.LeftLeg`) 0 "/Game/9_ShootingRange/Materials/MI_FlatColor_Brown.MI_FlatColor_Brown")
      (`PrimitiveComponent.SetMaterial` (`self.RightLeg`) 0 "/Game/9_ShootingRange/Materials/MI_FlatColor_Brown.MI_FlatColor_Brown")
      (`PrimitiveComponent.SetMaterial` (`self.RightLeg4`) 0 "/Game/9_ShootingRange/Materials/MI_FlatColor_Brown.MI_FlatColor_Brown")
      (`PrimitiveComponent.SetMaterial` (`self.RightLeg3`) 0 "/Game/9_ShootingRange/Materials/MI_FlatColor_Brown.MI_FlatColor_Brown")
      (`PrimitiveComponent.SetMaterial` (`self.RightLeg2`) 0 "/Game/9_ShootingRange/Materials/MI_FlatColor_Brown.MI_FlatColor_Brown")
      (`PrimitiveComponent.SetMaterial` (`self.LeftLeg1`) 0 "/Game/9_ShootingRange/Materials/MI_FlatColor_Brown.MI_FlatColor_Brown")
      (for _array_element_2 (`self.WeakPoints`)
        (`/Game/0_Design/EyeVisionSystem/BP_WeakPoints.Disable` _array_element_2)))))

(fn `EnableWeakPoints`
  (params (PlayerCamera :type "CineCameraComponent Object Reference")))

(fn `UserConstructionScript`)