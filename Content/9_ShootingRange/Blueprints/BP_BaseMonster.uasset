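; Base monster Blueprint for the shooting range that prepares its meshes and weak points at BeginPlay.
; It walks all descendant components of the root, setting every static mesh to block custom channel GameTraceChannel3.
; The same pass gathers BP_WeakPoints actors from Child Actor components into a unique WeakPoints array, so weak points are discovered from the component hierarchy.
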(event `self.ReceiveBeginPlay`
  ;[0.3302 0.0085 0 0.33] DEBUG
  (for _array_element (`SceneComponent.GetChildrenComponents` (`self.DefaultSceneRoot`) true)
    (`|ExecutionSequence`
      (:`then_0`
        (bind _asstatic_mesh_component (cast `StaticMeshComponent` _array_element))
        (`PrimitiveComponent.SetCollisionResponseToChannel` _asstatic_mesh_component "ECC_GameTraceChannel3" "ECR_Block"))
      (:`then_1`
        ;[1 1 1 0.33] Get all WeakPoints
        (bind _aschild_actor_component (cast `ChildActorComponent` _array_element))
        (bind _asbp_weak_points (cast `/Game/0_Design/EyeVisionSystem/BP_WeakPoints` (`ChildActorComponent.ChildActor` _aschild_actor_component)))
        (`KismetArrayLibrary.Array_AddUnique` (`self.WeakPoints`) _asbp_weak_points)))))

(fn `UserConstructionScript`)