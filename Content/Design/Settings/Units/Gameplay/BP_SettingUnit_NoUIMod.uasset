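; A gameplay setting unit for a "No UI Mod" toggle that hides parts of the in-game HUD.
; When applied in game, it finds the top-level WBP_Viewport widget and caches it.
; The boolean value zeroes or restores render opacity on the electricity and ammo counters, and collapses or shows the tutorial stack as hit-test invisible.
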(event `self.OnApplySetting`
  (params (bInGame :type Boolean))
  (bind _wbp_viewport (`self.WBP_Viewport`))
  (bind _wbp_electricitycounter (`/Game/Design/Widgets/WBP_Viewport.WBP_ElectricityCounter` _wbp_viewport))
  (bind _wbp_ammocounter (`/Game/Design/Widgets/WBP_Viewport.WBP_AmmoCounter` _wbp_viewport))
  (bind _tutorialactivatablestack (`/Game/Design/Widgets/WBP_Viewport.TutorialActivatableStack` _wbp_viewport))
  (if bInGame
    (`/Engine/EditorBlueprintResources/StandardMacros.IsValid` _wbp_viewport
      (:`Is Valid`
        _)
      (:`Is Not Valid`
        (bind _foundwidgets (`WidgetBlueprintLibrary.GetAllWidgetsOfClass` "/Game/Design/Widgets/WBP_Viewport.WBP_Viewport_C"))
        (set `self.WBP_Viewport` (`|GetArrayItem` _foundwidgets))))
    (if (`self.bValue`)
      (`Widget.SetRenderOpacity` _wbp_electricitycounter 0.0)
      (`Widget.SetRenderOpacity` _wbp_ammocounter 0.0)
      (`Widget.SetVisibility` _tutorialactivatablestack "Collapsed")
      (else
        (`Widget.SetRenderOpacity` _wbp_electricitycounter 1.0)
        (`Widget.SetRenderOpacity` _wbp_ammocounter 1.0)
        (`Widget.SetVisibility` _tutorialactivatablestack "HitTestInvisible")))))