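; An EQS testing pawn for the Parasite enemy that stands in as the querier when testing its environment queries.
; It supplies its own location as the query start and the PlayerStart tagged "Start" as the target, falling back to the first PlayerStart found.
; Target lookups print a testing-only warning, and a very short life span set on BeginPlay removes the pawn almost immediately during play.
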(event `self.ReceiveBeginPlay`
  (`self.SetLifeSpan` 0.1))

(fn `GetEQSStartLocation`
  (returns (ReturnValue :type "Vector Structure"))
  (return (`self.K2_GetActorLocation`)))

(fn `GetEQSTargetActor`
  (returns (ReturnValue :type "Actor Object Reference"))
  ;[1 1 1 0.33] Testing Purpose Only
  (`KismetSystemLibrary.PrintString` "BP_Parasite_EQSTestingPawn: testing purpose only!" true true (struct :`G` 0.66 :`B` 1.0 :`A` 1.0) 2.0 "EQSTestingPawn_Parasite")
  (bind _outactors (`GameplayStatics.GetAllActorsOfClass` "/Script/Engine.PlayerStart"))
  (for _array_element _outactors
    (if (== (`PlayerStart.PlayerStartTag` _array_element) "Start")
      (return _array_element)))
  (return (`|GetArrayItem` _outactors)))

(fn `UserConstructionScript`)