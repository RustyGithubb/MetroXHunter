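; Gears of War-style active reload QTE for the player's gun, with its own UI widget.
; A looping timer advances the reload cursor, and a second reload press is judged against timing windows as Perfect, Active or Failed.
; No press gives a normal reload, while perfect adds bonus ammo and failure adds a delay and sets a separate ammo count.
; Dispatchers and normalized getters expose state and timings; the perfect fire-rate boost is still TODO.
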(event `self.ReceiveBeginPlay`
  ;[1 0 0 0.33] BEGIN PLAY
  (`self.UpdateAmmoCount` (`/Game/0_Design/GameManagement_/BP_Gun.MaxMagazinAmmo` (`self.Gun`)))
  (`self.CreateWidget`))

(event `self.ReceiveEndPlay`
  (params (EndPlayReason :type "EEndPlayReason Enum" :default "Destroyed"))
  ;[1 0.2519 0 0.33] REMOVE WIDGET
  (`Widget.RemoveFromParent` (`self.Widget`)))

(event `StartReloadSequence`
  (if (not (`self.IsLockingGunFire`))
    (set `self.IsReloadActive` true)
    (set `self.CurrentGunState` "NewEnumerator2")
    (`self.UpdateCurrentReloadState` "NewEnumerator0")
    (set `self.ReloadElapsedTime` 0.0)
    (bind _returnvalue (`KismetSystemLibrary.K2_SetTimerDelegate` (delegate `UpdateReloadGauge`) (`self.ReloadRefreshRate`) true))
    (set `self.TimerHandleReloadPlayback` _returnvalue)))

(event `UpdateReloadGauge`
  (set `self.ReloadElapsedTime` (+ (`self.ReloadElapsedTime`) (`self.ReloadRefreshRate`)))
  (`self.OnUpdateCursorPosition`)
  ;[0 1 0.9093] Normal Reload if the player don't trigger the button
  (if (>= (`self.ReloadElapsedTime`) (`self.NormalReloadDuration`))
    (`KismetSystemLibrary.K2_ClearAndInvalidateTimerHandle` (`self.TimerHandleReloadPlayback`))
    (`self.TriggerNormalReload`)
    (set `self.IsReloadActive` false)))

(event `TriggerNormalReload`
  ;[0 1 0.9093] Normal Reload
  (`self.FinalizeReload` (`/Game/0_Design/GameManagement_/BP_Gun.MaxMagazinAmmo` (`self.Gun`)))
  (`self.UpdateCurrentReloadState` "NewEnumerator1"))

(event `TriggerActiveReload`
  ;[0 1 0.9093] Active Reload
  (`self.FinalizeReload` (`/Game/0_Design/GameManagement_/BP_Gun.MaxMagazinAmmo` (`self.Gun`)) "NewEnumerator3" (- (`self.ActiveReloadEndTime`) (`self.ReloadElapsedTime`)))
  (`self.UpdateCurrentReloadState` "NewEnumerator4"))

(event `TriggerPerfectReload`
  ;[0 1 0.9093] Perfect Reload
  (`self.FinalizeReload` (+ (`/Game/0_Design/GameManagement_/BP_Gun.MaxMagazinAmmo` (`self.Gun`)) (`self.PerfectBonusAmmo`)) "NewEnumerator5" (- (`self.ActiveReloadStartTime`) (`self.ReloadElapsedTime`)))
  ;;[1 1 1] TODO : Increase Fire Rate
  (`KismetSystemLibrary.Delay` (`self.PerfectReloadBonusTime`))
  (`self.UpdateCurrentReloadState` "NewEnumerator6"))

(event `TriggerFailedReload`
  ;[0 1 0.9093] Failed Reload
  (`self.FinalizeReload` (`self.FailedReloadAmmoCount`) "NewEnumerator7" (+ (- (`self.NormalReloadDuration`) (`self.ReloadElapsedTime`)) (`self.FailedReloadPenaltyTime`)))
  (`self.UpdateCurrentReloadState` "NewEnumerator8"))

(fn `CreateWidget`
  (bind _asbpc_controller (cast `/Game/0_Design/GameManagement_/BPC_Controller` (`Pawn.GetController` (`self.PlayerCharacter`))))
  (bind _returnvalue (`|CreateWidget` "/Game/UI/Widgets/ReloadSystem/WBP_ReloadSystem_QTE_MainUI.WBP_ReloadSystem_QTE_MainUI_C" _asbpc_controller))
  (bind _output_get (set `self.Widget` _returnvalue))
  (`UserWidget.AddToViewport` _output_get 0))

(fn `GetAmmoData`
  (returns (IndexMagazinAmmo :type Integer) (MaxMagazinAmmo :type Integer) (PerfectBonusAmmo :type Integer))
  (bind _gun (`self.Gun`))
  (return (`/Game/0_Design/GameManagement_/BP_Gun.IndexMagazinAmmo` _gun) (`/Game/0_Design/GameManagement_/BP_Gun.MaxMagazinAmmo` _gun) (`self.PerfectBonusAmmo`)))

(fn `GetCurrentReloadState`
  (returns (CurrentReloadState :type "/Game/0_Design/ReloadSystem/Enums/ENUM_PrimaryGunReloadState Enum"))
  (return (`self.CurrentReloadState`)))

(fn `GetNormalizedReloadElapsedTime`
  (returns (ReloadElapsedTime :type "Float (double-precision)"))
  (return (/ (`self.ReloadElapsedTime`) (`self.NormalReloadDuration`))))

(fn `GetNormalizedReloadTimings`
  (returns (PerfectReloadStartTime :type "Float (double-precision)") (ActiveReloadStartTime :type "Float (double-precision)") (ActiveReloadEndTime :type "Float (double-precision)"))
  (bind _normalreloadduration (`self.NormalReloadDuration`))
  (return (/ (`self.PerfectReloadStartTime`) _normalreloadduration) (/ (`self.ActiveReloadStartTime`) _normalreloadduration) (/ (`self.ActiveReloadEndTime`) _normalreloadduration)))

(fn `IsAmmoFull`
  (returns (ReturnValue :type Boolean))
  (bind _gun (`self.Gun`))
  (return (== (`/Game/0_Design/GameManagement_/BP_Gun.MaxMagazinAmmo` _gun) (`/Game/0_Design/GameManagement_/BP_Gun.IndexMagazinAmmo` _gun))))

(fn `IsLockingGunFire`
  (returns (IsFireLocked :type Boolean))
  (return (`self.IsReloadActive`)))

(fn `OnReloadInput`
  (params (`Input Type` :type "/Game/0_Design/ENUM_InputActionType Enum" :default "NewEnumerator0"))
  (if (`self.IsAmmoFull`)
    (`KismetSystemLibrary.PrintText` "FULL AMMO")
    (else
      (switch `/Game/0_Design/ENUM_InputActionType` `Input Type`
        (:`NewEnumerator1`
          (switch `/Game/0_Design/ReloadSystem/Enums/ENUM_PrimaryGunState` (`self.CurrentGunState`)
            (:`NewEnumerator0`
              (`self.StartReloadSequence`))
            (:`NewEnumerator2`
              ;[1 1 1] Based on the timing of triggering the reload, we defined if it is a Failed Reload, a Perfect Reload or an Active Reload
              (`KismetSystemLibrary.K2_ClearAndInvalidateTimerHandle` (`self.TimerHandleReloadPlayback`))
              (if (`KismetMathLibrary.InRange_FloatFloat` (`self.ReloadElapsedTime`) (`self.PerfectReloadStartTime`) (`self.ActiveReloadEndTime`))
                (if (< (`self.ReloadElapsedTime`) (`self.ActiveReloadStartTime`))
                  (`self.TriggerPerfectReload`)
                  (set `self.IsReloadActive` false)
                  (else
                    (`self.TriggerActiveReload`)
                    (set `self.IsReloadActive` false)))
                (else
                  (`self.TriggerFailedReload`)
                  (set `self.IsReloadActive` false))))))))))

(fn `UpdateAmmoCount`
  (params (NewCount :type Integer))
  (returns (Output_Get :type Integer))
  (bind _gun (`self.Gun`))
  (bind _output_get (set `/Game/0_Design/GameManagement_/BP_Gun.IndexMagazinAmmo` NewCount _gun))
  (`/Game/0_Design/GameManagement_/BP_Gun.OnFire` _gun)
  (return _output_get))

(fn `UpdateCurrentReloadState`
  (params (NewState :type "/Game/0_Design/ReloadSystem/Enums/ENUM_PrimaryGunReloadState Enum" :default "NewEnumerator0"))
  (set `self.CurrentReloadState` NewState)
  (`self.OnReloadStateUpdated`))