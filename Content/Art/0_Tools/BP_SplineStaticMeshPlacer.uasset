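; Editor placement tool that scatters copies of one static mesh along a spline in its construction script.
; It steps along the spline at Perlin-noise spacing driven by a seed, up to an iteration cap.
; Optional auto-snap line-traces from each point, moving the mesh to the hit and aligning it to the normal.
; Rotation offsets and random rotation and scale are then applied; these random values ignore the seed.
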(fn `ModifyStaticMeshTransform`
  (params (Transform :type "Transform Structure"))
  (returns (Result :type "Transform Structure"))
  (bind _outtransform (`self.ModifyTransformBySnapping` (`KismetMathLibrary.MakeTransform` Transform_Location (`KismetMathLibrary.ComposeRotators` Transform_Rotation (`self.SnapRotation`)) Transform_Scale)))
  (return (`KismetMathLibrary.MakeTransform` (.location _outtransform) (`KismetMathLibrary.ComposeRotators` (.rotation _outtransform) (`self.RotationOffset`)) (.scale _outtransform))))

(fn `ModifyTransformBySnapping`
  (params (Transform :type "Transform Structure"))
  (returns (OutTransform :type "Transform Structure"))
  (locals (NewLocation :type "Vector Structure"))
  (bind (_transform_location _transform_rotation _transform_scale) (`KismetMathLibrary.BreakTransform` (`local.Transform`)))
  (if (`self.bAutoSnap`)
    (bind (_outhit _returnvalue) (`KismetSystemLibrary.LineTraceSingle` :`Start` Transform_Location :`End` (+ Transform_Location (* (`KismetMathLibrary.NegateVector` (`KismetMathLibrary.GetForwardVector` Transform_Rotation)) (`self.SnapDistance`))) :`TraceChannel` "TraceTypeQuery1" :`DrawDebugType` "ForDuration"))
    (if _returnvalue
      (bind (_bblockinghit _binitialoverlap _time _distance _location _impactpoint _normal) (`GameplayStatics.BreakHitResult` _outhit))
      (return (`KismetMathLibrary.MakeTransform` _location (`KismetMathLibrary.Conv_VectorToRotator` _normal) _transform_scale))
      (else
        _)))
  (return (`KismetMathLibrary.MakeTransform` _transform_location _transform_rotation _transform_scale)))

(fn `RandomFloatFromSeed`
  (params (Item :type Integer) (Range :type "FloatRange Structure"))
  (returns (ReturnValue :type "Float (double-precision)"))
  (return (`KismetMathLibrary.MapRangeUnclamped` (`KismetMathLibrary.PerlinNoise1D` (+ (* (`self.Seed`) 0.01) (* Item 500.0))) -1.0 1.0 (`.Value` (break `FloatRangeBound` (break `FloatRange` Range))) (`.Value` (break `FloatRangeBound` (`.UpperBound` (break `FloatRange` Range)))))))

(fn `UserConstructionScript`
  (bind _returnvalue (`self.GetTransform`))
  (bind (_randomrotationoffset_roll _randomrotationoffset_pitch _randomrotationoffset_yaw) (`KismetMathLibrary.BreakRotator` (`self.RandomRotationOffset`)))
  (`self.StaticMesh`
    (:`then`
      (for _index (range (+ (`self.MaxIterations`) 1))
        (if (< (`self.CurrentDistance`) (`SplineComponent.GetSplineLength` (`self.Spline`)))
          (`|ExecutionSequence`
            (:`then_0`
              (bind _result (`self.ModifyStaticMeshTransform` (`SplineComponent.GetTransformAtDistanceAlongSpline` (`self.Spline`) (`self.CurrentDistance`) "World" false)))
              (bind _returnvalue_2 (`AddComponent|NODE_AddStaticMeshComponent-1` :`RelativeTransform` (`KismetMathLibrary.MakeTransform` (`KismetMathLibrary.InverseTransformLocation` _returnvalue (.location _result)) (`KismetMathLibrary.ComposeRotators` (`KismetMathLibrary.InverseTransformRotation` _returnvalue (.rotation _result)) (`KismetMathLibrary.MakeRotator` (`KismetMathLibrary.RandomFloatInRange` (* _randomrotationoffset_roll -1.0) _randomrotationoffset_roll) (`KismetMathLibrary.RandomFloatInRange` (* _randomrotationoffset_pitch -1.0) _randomrotationoffset_pitch) (`KismetMathLibrary.RandomFloatInRange` (* _randomrotationoffset_yaw -1.0) _randomrotationoffset_yaw))) (* (.scale _result) (`KismetMathLibrary.Conv_DoubleToVector` (`UtilityLibrary.RandomInRange` (`self.ScaleRange`)))))))
              (`StaticMeshComponent.SetStaticMesh` _returnvalue_2 (`self.StaticMesh`)))
            (:`then_1`
              (`/Game/Design/Libraries/BPL_GeneralUtilities.Increase Value Float Clamped` (`self.CurrentDistance`) (`self.RandomFloatFromSeed` _index (`self.DistanceRange`)) 0.0 (`SplineComponent.GetSplineLength` (`self.Spline`)))))
          (else
            (break)))))
    (:`else`)))