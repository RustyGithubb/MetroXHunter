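; Settings unit Blueprint that applies the player's chosen aim assist level during gameplay.
; On apply in game, it finds the aim assist component on the first player pawn, waiting a tick first if it has no cached reference.
; It maps the selected index to a difficulty, stores it as the component's starting difficulty, then refreshes the component's aim assist settings.
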(event `self.OnApplySetting`
  (params (bInGame :type Boolean))
  (if bInGame
    (`/Engine/EditorBlueprintResources/StandardMacros.IsValid` (`self.AimAssistComponent`)
      (:`Is Valid`
        _)
      (:`Is Not Valid`
        (`KismetSystemLibrary.DelayUntilNextTick`)
        (bind _output_get (set `self.AimAssistComponent` (`Actor.GetComponentByClass` (`GameplayStatics.GetPlayerPawn` 0) "/AdvancedAimAssist/Blueprints/Components/AAA_BP_AimAssistComponent.AAA_BP_AimAssistComponent_C")))))
    (bind _output_get_2 (set `/AdvancedAimAssist/Blueprints/Components/AAA_BP_AimAssistComponent.StartingDifficulty` (`|GetArrayItem` (`self.AimDifficulty`) (`self.IndexValue`)) _output_get))
    (`/AdvancedAimAssist/Blueprints/Components/AAA_BP_AimAssistComponent.UpdateAimAssistSettings` _output_get _output_get_2)))