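; Blueprint function library for spawning Niagara or particle systems that feed the volumetric fog's 2D interaction.
; Two functions, one at a location and one attached, spawn the system only if the level's BP_FogInteractionController has a valid SceneCapture and 2D interaction enabled.
; Each spawned system joins that capture's show-only list and is visible only in scene captures.
; A third function returns the controller reference.
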(fn `FogVolumetricInteractionReference`
  (returns (InteractionControllerRef :type "/Game/Art/VFX/Volumetric_Fog/Blueprints/BP_FogInteractionController Object Reference"))
  (locals (InteractionControlRef :type "/Game/Art/VFX/Volumetric_Fog/Blueprints/BP_FogInteractionController Object Reference"))
  (bind _returnvalue (`GameplayStatics.GetActorOfClass` null "/Game/Art/VFX/Volumetric_Fog/Blueprints/BP_FogInteractionController.BP_FogInteractionController_C"))
  (`/Engine/EditorBlueprintResources/StandardMacros.IsValid` _returnvalue
    (:`Is Valid`
      (bind _output_get (set `local.InteractionControlRef` _returnvalue))
      (return _output_get))))

(fn `FogVolumetricSystem`
  (params (SystemTemplate :type "NiagaraSystem Object Reference") (Location :type "Vector Structure") (Rotation :type "Rotator Structure"))
  (returns (NSReference :type "NiagaraComponent Object Reference"))
  (bind _returnvalue (`GameplayStatics.GetActorOfClass` null "/Game/Art/VFX/Volumetric_Fog/Blueprints/BP_FogInteractionController.BP_FogInteractionController_C"))
  (`/Engine/EditorBlueprintResources/StandardMacros.IsValid` _returnvalue
    (:`Is Valid`
      (bind _scenecapture (`/Game/Art/VFX/Volumetric_Fog/Blueprints/BP_FogInteractionController.SceneCapture` _returnvalue))
      (if (and (`KismetSystemLibrary.IsValid` _scenecapture) (`/Game/Art/VFX/Volumetric_Fog/Blueprints/BP_FogInteractionController.Interaction2DEnable` _returnvalue))
        (bind _returnvalue_2 (`NiagaraFunctionLibrary.SpawnSystemAtLocation` null SystemTemplate Location Rotation))
        (`SceneCaptureComponent.ShowOnlyComponent` _scenecapture _returnvalue_2)
        (`PrimitiveComponent.SetVisibleInSceneCaptureOnly` _returnvalue_2 true)
        (return _returnvalue_2)))))

(fn `FogVolumetricSystemAttached`
  (params (SystemTemplate :type "NiagaraSystem Object Reference") (AttachToComponent :type "SceneComponent Object Reference") (Location :type "Vector Structure") (Rotation :type "Rotator Structure"))
  (returns (NSReference :type "NiagaraComponent Object Reference"))
  (bind _returnvalue (`GameplayStatics.GetActorOfClass` null "/Game/Art/VFX/Volumetric_Fog/Blueprints/BP_FogInteractionController.BP_FogInteractionController_C"))
  (`/Engine/EditorBlueprintResources/StandardMacros.IsValid` _returnvalue
    (:`Is Valid`
      (bind _scenecapture (`/Game/Art/VFX/Volumetric_Fog/Blueprints/BP_FogInteractionController.SceneCapture` _returnvalue))
      (if (and (`KismetSystemLibrary.IsValid` _scenecapture) (`/Game/Art/VFX/Volumetric_Fog/Blueprints/BP_FogInteractionController.Interaction2DEnable` _returnvalue))
        (bind _returnvalue_2 (`NiagaraFunctionLibrary.SpawnSystemAttached` SystemTemplate AttachToComponent "None" Location Rotation "SnapToTarget"))
        (`SceneCaptureComponent.ShowOnlyComponent` _scenecapture _returnvalue_2)
        (`PrimitiveComponent.SetVisibleInSceneCaptureOnly` _returnvalue_2 true)
        (return _returnvalue_2)))))