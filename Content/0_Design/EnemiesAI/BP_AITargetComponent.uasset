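; Actor component that gives its owner, as an AI target, a limited pool of tokens that other objects can reserve.
; A map stores tokens per reserver, and a reservation overwrites that reserver's entry only if enough tokens remain under MaxTokens.
; Reservers free tokens partially or entirely, and BeginPlay clears the map.
; Tick runs only with debug drawing enabled, showing the token count and reservations above the owner.
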(event `self.ReceiveBeginPlay`
  (`self.ResetTokens`)
  (`self.SetComponentTickEnabled` (`self.IsDrawDebugEnabled`)))

(event `self.ReceiveTick`
  (params (DeltaSeconds :type "Float (single-precision)"))
  (`KismetSystemLibrary.DrawDebugString` (+ (`Actor.K2_GetActorLocation` (`self.GetOwner`)) (0.0 0.0 75.0)) (`KismetTextLibrary.Conv_TextToString` (`|FormatText` "[AITargetComponent] \nTokens: {RemainingTokens}/{MaxTokens} \nReservations: \n{Reservations}" (`self.GetRemainingTokens`) (`self.MaxTokens`) (`self.FormatReservedTokens`))) null))

(fn `FormatReservedTokens`
  (returns (Text :type String))
  (locals (FormattedText :type String))
  (bind _reservedtokens (`self.ReservedTokens`))
  (bind _keys (`BlueprintMapLibrary.Map_Keys` _reservedtokens))
  (for _array_element _keys
    (set `local.FormattedText` (`KismetStringLibrary.Concat_StrStr` (`local.FormattedText`) (`KismetTextLibrary.Conv_TextToString` (`|FormatText` "- {Actor}: {Tokens} \n" _array_element (`BlueprintMapLibrary.Map_Find` _reservedtokens _array_element))))))
  (return (`local.FormattedText`)))

(fn `FreeAllTokens`
  (params (Reserver :type "Actor Object Reference"))
  (`BlueprintMapLibrary.Map_Remove` (`self.ReservedTokens`) Reserver))

(fn `FreeTokens`
  (params (Reserver :type "Actor Object Reference") (Tokens :type Integer))
  (bind _reservedtokens (`self.ReservedTokens`))
  (`BlueprintMapLibrary.Map_Add` _reservedtokens Reserver (`KismetMathLibrary.Max` (- (`BlueprintMapLibrary.Map_Find` _reservedtokens Reserver) Tokens))))

(fn `GetRemainingTokens`
  (returns (Tokens :type Integer))
  (locals (RemainingTokens :type Integer))
  (bind _remainingtokens (`local.RemainingTokens`))
  (bind _reservedtokens (`self.ReservedTokens`))
  (set `local.RemainingTokens` (`self.MaxTokens`))
  (bind _keys (`BlueprintMapLibrary.Map_Keys` _reservedtokens))
  (for _array_element _keys
    (`/Game/o_Libraries/BPL_GeneralUtilities.Decrease Value Int` _remainingtokens (`BlueprintMapLibrary.Map_Find` _reservedtokens _array_element)))
  (return _remainingtokens))

(fn `ReserveTokens`
  (params (Reserver :type "Actor Object Reference") (Tokens :type Integer))
  (returns (bIsSuccess :type Boolean))
  (`/Engine/EditorBlueprintResources/StandardMacros.IsValid` Reserver
    (:`Is Valid`
      (if (>= (`self.GetRemainingTokens`) Tokens)
        (`BlueprintMapLibrary.Map_Add` (`self.ReservedTokens`) Reserver (`local.Tokens`))
        (return true)
        (else
          (return false))))
    (:`Is Not Valid`
      (return false))))

(fn `ResetTokens`
  (`BlueprintMapLibrary.Map_Clear` (`self.ReservedTokens`)))