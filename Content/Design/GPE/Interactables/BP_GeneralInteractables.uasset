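; BP_GeneralInteractables is a general interactable actor that shows an on-screen prompt based on proximity and targeting.
; The outer collision shows or hides the widget component on any overlap.
; The inner collision finds the overlapping actor's InteractionComponent and reports entry and exit to its InteractableComponent.
; Targeting events drive the cached WBP_Interactable, collapsing its far widget when targeted and calling OnUntargeted when untargeted or on inner exit.
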(event `self.ReceiveBeginPlay`
  (`self.SetInteractableWidget`))

(event `self.InnerCollision.OnComponentBeginOverlap`
  (params (OverlappedComponent :type "PrimitiveComponent Object Reference") (OtherActor :type "Actor Object Reference") (OtherComp :type "PrimitiveComponent Object Reference") (OtherBodyIndex :type Integer) (bFromSweep :type Boolean) (SweepResult :type "HitResult Structure (by ref)"))
  (bind _returnvalue (`self.GetComponentByClass` OtherActor "/Script/MetroXHunter.InteractionComponent"))
  ;[1 1 1 0.33] OVERLAP INNER CIRCLE
  (`/Engine/EditorBlueprintResources/StandardMacros.IsValid` _returnvalue
    (:`Is Valid`
      (bind _output_get (set `self.PlayerInteractionComponent` _returnvalue))
      (`InteractableComponent.OnPlayerOverlap` (`self.InteractableComponent`) _output_get))))

(event `self.InnerCollision.OnComponentEndOverlap`
  (params (OverlappedComponent :type "PrimitiveComponent Object Reference") (OtherActor :type "Actor Object Reference") (OtherComp :type "PrimitiveComponent Object Reference") (OtherBodyIndex :type Integer))
  ;[1 1 1 0.33] END OVERLAP INNER CIRCLE
  (bind _playerinteractioncomponent (`self.PlayerInteractionComponent`)
    (:`then`
      (`InteractableComponent.OnPlayerOut` (`self.InteractableComponent`) _playerinteractioncomponent)
      (`/Game/Design/Widgets/WBP_Interactable.OnUntargeted` (`self.InteractableWidget`)))
    (:`else`)))

(event `self.OutterCollision.OnComponentBeginOverlap`
  (params (OverlappedComponent :type "PrimitiveComponent Object Reference") (OtherActor :type "Actor Object Reference") (OtherComp :type "PrimitiveComponent Object Reference") (OtherBodyIndex :type Integer) (bFromSweep :type Boolean) (SweepResult :type "HitResult Structure (by ref)"))
  ;[1 1 1 0.33] OVERLAP OUTTER CIRCLE
  (`SceneComponent.SetHiddenInGame` (`self.Widget`) false false))

(event `self.OutterCollision.OnComponentEndOverlap`
  (params (OverlappedComponent :type "PrimitiveComponent Object Reference") (OtherActor :type "Actor Object Reference") (OtherComp :type "PrimitiveComponent Object Reference") (OtherBodyIndex :type Integer))
  ;[1 1 1 0.33] END OVERLAP OUTTER CIRCLE
  (`SceneComponent.SetHiddenInGame` (`self.Widget`) true false))

(event `self.InteractableComponent.OnTargeted`
  ;[1 1 1 0.33] ON TARGETED
  (set `Widget.Visibility` "Collapsed" (`/Game/Design/Widgets/WBP_Interactable.FarWidget` (`self.InteractableWidget`))))

(event `self.InteractableComponent.OnUntargeted`
  ;[1 1 1 0.33] ON UNTARGETED
  (`/Game/Design/Widgets/WBP_Interactable.OnUntargeted` (`self.InteractableWidget`)))

(fn `SetInteractableWidget`
  (bind _aswbp_interactable (cast `/Game/Design/Widgets/WBP_Interactable` (`WidgetComponent.GetWidget` (`self.Widget`))))
  (set `self.InteractableWidget` _aswbp_interactable))

(fn `UserConstructionScript`)