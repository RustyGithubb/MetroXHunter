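; Destructible light actor that switches on and off with sound and supports flickering.
; BeginPlay caches light intensities and finds meshes using the Materials map, then switching zeroes or restores intensities and swaps those slots between black and mapped materials.
; Flicker callbacks drive emissive intensity, creating dynamic material instances on every update (flagged TODO).
; On death, unless child-overridden, it plays sparks and sound, respawns non-blacklisted meshes as unlit StaticMeshActors and destroys itself.
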(event `self.ReceiveBeginPlay`
  (`|ExecutionSequence`
    (:`then_0`
      ;[0 0 0 1 40] SET LIGHT EDITOR VIEW
      (for _array_element (`self.K2_GetComponentsByClass` "/Script/Engine.LightComponent")
        (`SceneComponent.SetVisibility` _array_element true false)))
    (:`then_1`
      ;[0 0 0 1 40] SET LIGHT ARRAY
      (for _array_element_2 (`self.K2_GetComponentsByClass` "/Script/Engine.LightComponent")
        (`BlueprintMapLibrary.Map_Add` (`self.LightIntensityPerComponent`) _array_element_2 (`LightComponentBase.Intensity` _array_element_2))))
    (:`then_2`
      (`self.Retrieve Light Static Meshes`)
      (`self.Actualise State Light` (`self.Should OFF`)))))

(event `self.Health.OnDeath`
  (params (DamageContext :type "DamageContext Structure (by ref)"))
  (if (not (`self.bIsOverrideByChild`))
    (`self.Explode / Destroy Himself` "/Game/Art/VFX/NS_Electrics/Gun/NS_Lightning_Sparks_Impact.NS_Lightning_Sparks_Impact")))

(fn `Actualise State Light`
  (params (`Should OFF` :type Boolean))
  (bind _output_get (set `self.Should OFF` `Should OFF`))
  (if _output_get
    ;[1 0 0 1 40] OFF
    (`self.Switch OFF`)
    (else
      ;[0.02518 0.3281 0 1 40] ON
      (`self.Switch ON`))))

(fn `Explode / Destroy Himself`
  (params (`Niagara System` :type "NiagaraSystem Object Reference"))
  (locals (`Niagara System ` :type "NiagaraSystem Object Reference" :default "/Script/Niagara.NiagaraSystem'/Game/Art/VFX/NS_Sparks/NS_Sparks_Lock_Stock.NS_Sparks_Lock_Stock'"))
  (bind (_returnvalue_location _returnvalue_rotation) (`KismetMathLibrary.BreakTransform` (`self.GetTransform`)))
  (`self.Set BlackList Component`)
  (`/Engine/EditorBlueprintResources/StandardMacros.IsValid` `Niagara System`
    (:`Is Valid`
      (set `local.Niagara System ` `Niagara System`))
    (:`Is Not Valid`
      _))
  ;[1 1 1 0.33] FEEDBACK
  (`GameplayStatics.PlaySoundAtLocation` "/Game/Sounds/Audio/SD/SoundWaves/GPE/Transformator/SW_GPE_Station_Transformator_Desactivation.SW_GPE_Station_Transformator_Desactivation" (`self.K2_GetActorLocation`) (struct) 1.0 1.0 0.0 (`self.Attenuation Settings`) null null null)
  (`NiagaraFunctionLibrary.SpawnSystemAtLocation` (`local.Niagara System `) _returnvalue_location _returnvalue_rotation (5.0 5.0 5.0))
  ;[1 0 0 0.33] RESPAWN
  (`self.Respawn StaticMesh`)
  (`self.K2_DestroyActor`))

(fn `OnFlickLightStart`
  (params (LightData :type "LightData Structure (by ref)"))
  (bind _lightintensitypercomponent (`self.LightIntensityPerComponent`))
  (if (not (`self.IsDead`))
    (`self.Switch Materials to` "/Game/Art/0_Materials/Material_Instance/MI_Neon_White_lumen.MI_Neon_White_lumen")
    (if (not (`BlueprintMapLibrary.Map_IsEmpty` (`self.LightIntensityPerComponent`)))
      (bind _keys (`BlueprintMapLibrary.Map_Keys` _lightintensitypercomponent))
      (for _array_element _keys
        (bind (_value _returnvalue) (`BlueprintMapLibrary.Map_Find` _lightintensitypercomponent _array_element))
        (if _returnvalue
          (setmembers `LightData` :`StructRef` LightData :`OriginalLightIntensity` _value)))
      (return))))

(fn `OnFlickLightStop`
  (params (LightData :type "LightData Structure (by ref)"))
  (if (not (`self.IsDead`))
    (`self.Actualise State Light` (`self.Should OFF`))
    (return)))

(fn `OnFlickLightTick`
  (params (DeltaTime :type "Float (single-precision)") (LightData :type "LightData Structure (by ref)"))
  (return))

(fn `OnFlickLightUpdate`
  (params (LightData :type "LightData Structure (by ref)") (IntensityScale :type "Float (single-precision)"))
  (if (not (`self.IsDead`))
    (`self.Set Emissive Value ` IntensityScale)
    (return)))

(fn `Respawn StaticMesh`
  (locals (`Static Mesh Can be Respawn` :type Boolean :default true) (`Actual Static mesh` :type "StaticMeshComponent Object Reference") (MaterialsKeys :type "Array of Integer"))
  (bind (_returnvalue_location _returnvalue_rotation _returnvalue_scale) (`KismetMathLibrary.BreakTransform` (`SceneComponent.K2_GetComponentToWorld` (`local.Actual Static mesh`))))
  (`|ExecutionSequence`
    (:`then_0`
      (bind _keys (`BlueprintMapLibrary.Map_Keys` (`self.Materials`)))
      (set `local.MaterialsKeys` _keys))
    (:`then_1`
      (for _array_element (`self.K2_GetComponentsByClass` "/Script/Engine.StaticMeshComponent")
        (bind _output_get (set `local.Actual Static mesh` _array_element))
        (for _array_element_2 (`self.BlackListComp`)
          (if (== _array_element_2 _output_get)
            (set `local.Static Mesh Can be Respawn` false)
            (break)
            (else
              (set `local.Static Mesh Can be Respawn` true))))
        (if (`local.Static Mesh Can be Respawn`)
          (bind _returnvalue (`|SpawnActorFromClass` "/Script/Engine.StaticMeshActor" (`KismetMathLibrary.MakeTransform` _returnvalue_location _returnvalue_rotation _returnvalue_scale) "AlwaysSpawn" "MultiplyWithRoot" null null))
          (`StaticMeshActor.SetMobility` _returnvalue "Stationary")
          (bind _staticmeshcomponent (`StaticMeshActor.StaticMeshComponent` _returnvalue))
          (`UtilityLibrary.SetActorComponentCanEverAffectNavigation` _staticmeshcomponent)
          (`StaticMeshComponent.SetStaticMesh` _staticmeshcomponent (`StaticMeshComponent.StaticMesh` (`local.Actual Static mesh`)))
          ;[1 1 1 0.33] SET EMISSIVE LIGHT
          (bind _returnvalue_2 (`PrimitiveComponent.CreateDynamicMaterialInstance` _staticmeshcomponent (`|GetArrayItem` (`local.MaterialsKeys`)) (`BlueprintMapLibrary.Map_Find` (`self.Materials`)) "None"))
          (`/Engine/EditorBlueprintResources/StandardMacros.IsValid` _returnvalue_2
            (:`Is Valid`
              (`MaterialInstanceDynamic.SetScalarParameterValue` _returnvalue_2 (`self.Parameter Name`) 0.0)))))
      (return))))

(fn `Retrieve Light Static Meshes`
  (`KismetArrayLibrary.Array_Clear` (`self.LightStaticMeshes`))
  (for _array_element (`self.K2_GetComponentsByClass` "/Script/Engine.StaticMeshComponent")
    (for _array_element_2 (`MeshComponent.GetMaterials` _array_element)
      (bind _values (`BlueprintMapLibrary.Map_Values` (`self.Materials`)))
      (for _array_element_3 _values
        (if (== _array_element_3 _array_element_2)
          (`KismetArrayLibrary.Array_Add` (`self.LightStaticMeshes`) _array_element))))))

(fn `RetrieveFlickableLights`
  (returns (ReturnValue :type "Array of LightComponent Object Reference"))
  (bind _keys (`BlueprintMapLibrary.Map_Keys` (`self.LightIntensityPerComponent`)))
  (return _keys))

(fn `Set BlackList Component`
  (for _array_element (`self.K2_GetComponentsByClass` "/Script/Engine.StaticMeshComponent")
    (for _array_element_2 (`ActorComponent.ComponentTags` _array_element)
      (if (== _array_element_2 (`self.Black List Tag`))
        (`KismetArrayLibrary.Array_Add` (`self.BlackListComp`) _array_element)))))

(fn `Set Emissive Value `
  (params (`Light Multiplier emissive` :type "Float (double-precision)"))
  (bind _materials (`self.Materials`))
  ;[0 0 0 1 40] Emissive Intensity
  (if (not (`BlueprintMapLibrary.Map_IsEmpty` (`self.Materials`)))
    (for _array_element (`self.LightStaticMeshes`)
      (bind _keys (`BlueprintMapLibrary.Map_Keys` _materials))
      (for _array_element_2 _keys
        (bind (_value _returnvalue) (`BlueprintMapLibrary.Map_Find` _materials _array_element_2))
        (if _returnvalue
          (bind _returnvalue_2 (`PrimitiveComponent.CreateDynamicMaterialInstance` _array_element _array_element_2 _value "None" :!pinned true)) ; TODO: Optimize this, creating a dynamic material for each static mesh each call seems very bad.
          (`MaterialInstanceDynamic.SetScalarParameterValue` _returnvalue_2 "Emissive Intensity" (* `Light Multiplier emissive` 25.0)))))))

(fn `Switch Materials to`
  (params (InputPin :type "MaterialInterface Object Reference"))
  (bind _materials (`self.Materials`))
  ;[0 0 0 1 40] SWITCH ON
  (if (not (`BlueprintMapLibrary.Map_IsEmpty` (`self.Materials`)))
    (for _array_element (`self.LightStaticMeshes`)
      (bind _keys (`BlueprintMapLibrary.Map_Keys` _materials))
      (for _array_element_2 _keys
        (if (`.ReturnValue` (`BlueprintMapLibrary.Map_Find` _materials _array_element_2))
          (`PrimitiveComponent.SetMaterial` _array_element _array_element_2 InputPin))))))

(fn `Switch OFF`
  (locals (MaterialsKeys :type "Array of Integer"))
  (bind _lightintensitypercomponent (`self.LightIntensityPerComponent`))
  (`GameplayStatics.PlaySoundAtLocation` "/Game/Sounds/Audio/SD/MetaSounds/MS_Sources/SFX/MS_SFX_LightsSwitch.MS_SFX_LightsSwitch" (`self.K2_GetActorLocation`) (struct) 1.0 1.0 0.0 "/Game/Sounds/Audio/SD/Att/Att_20m.Att_20m" null null null)
  (`|ExecutionSequence`
    (:`then_0`
      ;[1 0 0 1 40] SWITCH OFF
      (bind _keys (`BlueprintMapLibrary.Map_Keys` (`self.Materials`)))
      (set `local.MaterialsKeys` _keys)
      (if (not (`BlueprintMapLibrary.Map_IsEmpty` (`self.Materials`)))
        (for _array_element (`self.LightStaticMeshes`)
          (for _array_element_2 (`local.MaterialsKeys`)
            (if (`.ReturnValue` (`BlueprintMapLibrary.Map_Find` (`self.Materials`) _array_element_2))
              (`PrimitiveComponent.SetMaterial` _array_element _array_element_2 "/AdvancedAimAssist/DemoContent/Materials/MI_TileBlack.MI_TileBlack"))))))
    (:`then_1`
      (if (not (`BlueprintMapLibrary.Map_IsEmpty` (`self.LightIntensityPerComponent`)))
        (bind _keys_2 (`BlueprintMapLibrary.Map_Keys` _lightintensitypercomponent))
        (for _array_element_3 _keys_2
          (if (`.ReturnValue` (`BlueprintMapLibrary.Map_Find` _lightintensitypercomponent _array_element_3))
            (`LightComponent.SetIntensity` _array_element_3 0.0)))))))

(fn `Switch ON`
  (bind _materials (`self.Materials`))
  (bind _lightintensitypercomponent (`self.LightIntensityPerComponent`))
  (`GameplayStatics.PlaySoundAtLocation` "/Game/Sounds/Audio/SD/MetaSounds/MS_Sources/SFX/MS_SFX_LightsSwitch.MS_SFX_LightsSwitch" (`self.K2_GetActorLocation`) (struct) 1.0 1.0 0.0 "/Game/Sounds/Audio/SD/Att/Att_20m.Att_20m" null null null)
  (`|ExecutionSequence`
    (:`then_0`
      ;[0.02518 0.3281 0 1 40] SWITCH ON
      (if (not (`BlueprintMapLibrary.Map_IsEmpty` (`self.Materials`)))
        (for _array_element (`self.LightStaticMeshes`)
          (bind _keys (`BlueprintMapLibrary.Map_Keys` _materials))
          (for _array_element_2 _keys
            (bind (_value _returnvalue) (`BlueprintMapLibrary.Map_Find` _materials _array_element_2))
            (if _returnvalue
              (`PrimitiveComponent.SetMaterial` _array_element _array_element_2 _value))))))
    (:`then_1`
      (if (not (`BlueprintMapLibrary.Map_IsEmpty` (`self.LightIntensityPerComponent`)))
        (bind _keys_2 (`BlueprintMapLibrary.Map_Keys` _lightintensitypercomponent))
        (for _array_element_3 _keys_2
          (bind (_value_2 _returnvalue_2) (`BlueprintMapLibrary.Map_Find` _lightintensitypercomponent _array_element_3))
          (if _returnvalue_2
            (`LightComponent.SetIntensity` _array_element_3 _value_2)))))))

(fn `UserConstructionScript`
  ;[0 0 0 1 40] SET LIGHT EDITOR VIEW
  (for _array_element (`self.K2_GetComponentsByClass` "/Script/Engine.LightComponent")
    (`SceneComponent.SetVisibility` _array_element (not (`self.Should OFF`)) false)))