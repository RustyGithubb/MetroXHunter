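; Parent Blueprint for stairs that pair a visible stairs mesh with a ramp collider toggled by main character run events.
; When flagged elevated, the construction script swaps in elevated ramp and stairs meshes, printing an error if either is invalid.
; A gameplay-tag event handler enables ramp collision on StartRun and disables it on StopRun, although BeginPlay binds only StartRun.
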(event `self.ReceiveBeginPlay`
  (`/EventDispatcherHub/FunctionLibrary/BPL_EventDispatcherHub.Bind to Multiple Gameplay Events` (struct :`GameplayTags` (struct :`(TagName` "Event.mainCharacter.StartRun") :`(TagName` "Event.mainCharacter.StopRun"))) self))

(fn `ReceiveEvent`
  (params (CalledTag :type "GameplayTag Structure") (CallingObject :type "Object Object Reference (by ref)"))
  (returns (Return :type Boolean))
  (bind _rampcollider (`self.RampCollider`))
  (`|SwitchGameplayTag` CalledTag
    (:`Default`
      (return false))
    (:`Event.mainCharacter.StartRun`
      (`PrimitiveComponent.SetCollisionEnabled` _rampcollider "QueryAndPhysics"))
    (:`Event.mainCharacter.StopRun`
      (`PrimitiveComponent.SetCollisionEnabled` _rampcollider "NoCollision"))))

(fn `UserConstructionScript`
  (if (`self.bIsElevated`)
    (`|ExecutionSequence`
      (:`then_0`
        (bind _elevatedrampmesh (`self.ElevatedRampMesh`)
          (:`then`
            (`StaticMeshComponent.SetStaticMesh` (`self.RampCollider`) _elevatedrampmesh))
          (:`else`
            (`KismetSystemLibrary.PrintString` "Stairs : Y'a pas de elevated mesh connard" true true (struct :`R` 1.0 :`B` 0.041656 :`A` 1.0) 2.0 "0" :!label _label))))
      (:`then_1`
        (bind _elevatedstairsmesh (`self.ElevatedStairsMesh`)
          (:`then`
            (`StaticMeshComponent.SetStaticMesh` (`self.StairsMesh`) _elevatedstairsmesh))
          (:`else`
            (goto _label)))))))