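; Trigger receiver component that plays, stops or triggers atmosphere sound in response to trigger box events.
; The configured action selects behavior on box enter; only the paired Play and Stop/Trigger actions also react on exit.
; Play prefers the referenced AmbientSound, falling back to spawning the sound asset in 2D or at the owner's location.
; The stored audio component receives later trigger parameters and stops, with optional fade-out.
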(event `self.ReceiveBeginPlay`
  (bind (_details_action _details_ambientsound) (break `SoundAtmosphereDetails` (`self.Details`)))
  (`/Engine/EditorBlueprintResources/StandardMacros.IsValid` _details_ambientsound
    (:`Is Valid`
      (set `self.PlayingAudioComponent` (`AmbientSound.AudioComponent` _details_ambientsound)))))

(fn `OnPlayComponentSpecificEvent`
  (params (FromBoxEnter :type Boolean) (TriggerBox :type "Actor Object Reference"))
  (bind _details_action (break `SoundAtmosphereDetails` (`self.Details`)))
  (if FromBoxEnter
    (switch `ESoundAtmosphereActionType` _details_action
      (:`PlayAndStop`
        (if FromBoxEnter :!label _label
          (`self.PlaySound`)
          (else
            (`self.StopSound`))))
      (:`PlayAndTrigger`
        (if FromBoxEnter :!label _label_2
          (`self.PlaySound`)
          (else
            (`self.TriggerSound`))))
      (:`Play`
        (`self.PlaySound`))
      (:`Trigger`
        (`self.TriggerSound`))
      (:`Stop`
        (`self.StopSound`)))
    (else
      (switch `ESoundAtmosphereActionType` _details_action
        (:`PlayAndStop`
          (goto _label))
        (:`PlayAndTrigger`
          (goto _label_2))))))

(fn `PlaySound`
  (bind (_details_action _details_ambientsound _details_soundasset _details_bisplaying2d) (break `SoundAtmosphereDetails` (`self.Details`)))
  (bind _audiocomponent (`AmbientSound.AudioComponent` _details_ambientsound))
  (`/Engine/EditorBlueprintResources/StandardMacros.IsValid` _details_ambientsound
    (:`Is Valid`
      (`AudioComponent.Play` _audiocomponent 0.0)
      (set `self.PlayingAudioComponent` _audiocomponent))
    (:`Is Not Valid`
      (`/Engine/EditorBlueprintResources/StandardMacros.IsValid` _details_soundasset
        (:`Is Valid`
          (if _details_bisplaying2d
            (bind _returnvalue (`GameplayStatics.SpawnSound2D` _details_soundasset 1.0 1.0 0.0 null))
            (set `self.PlayingAudioComponent` _returnvalue)
            (else
              (bind _returnvalue_2 (`GameplayStatics.SpawnSoundAtLocation` _details_soundasset (`Actor.K2_GetActorLocation` (`self.GetOwner`)) (struct) 1.0 1.0 0.0 null null))
              (set `self.PlayingAudioComponent` _returnvalue_2))))
        (:`Is Not Valid`
          (`KismetSystemLibrary.PrintText` (`|FormatText` "BP_SoundAtmosphereTriggerReceiver_Component: {Owner} don't have a valid sound to play, please reference one!" (`KismetSystemLibrary.GetDisplayName` (`self.GetOwner`))) true true (struct :`R` 1.0 :`A` 1.0) 10.0))))))

(fn `StopSound`
  (bind _playingaudiocomponent (`self.PlayingAudioComponent`))
  (bind (_details_action _details_ambientsound _details_soundasset _details_bisplaying2d _details_triggerparameter _details_fadeouttime) (break `SoundAtmosphereDetails` (`self.Details`)))
  (if (> _details_fadeouttime 0.0)
    (`AudioComponent.FadeOut` _playingaudiocomponent _details_fadeouttime 0.0 "Linear")
    (else
      (`AudioComponent.Stop` _playingaudiocomponent))))

(fn `TriggerSound`
  (bind (_details_action _details_ambientsound _details_soundasset _details_bisplaying2d _details_triggerparameter) (break `SoundAtmosphereDetails` (`self.Details`)))
  (`AudioParameterControllerInterface.SetTriggerParameter` (`self.PlayingAudioComponent`) _details_triggerparameter))