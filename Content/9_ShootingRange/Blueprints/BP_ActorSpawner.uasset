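; Shooting range spawner that periodically spawns a configurable actor class at its own transform, up to a maximum live count.
; A looping timer spawns while the tracked Actors array is below MaxActors, and each actor's OnEndPlay removes it, freeing a slot.
; Spawned pawns get a default controller if needed.
; Optional NoGravity zeroes CharacterMovement gravity; actors lacking that component then print an error and go untracked.
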(event `self.ReceiveBeginPlay`
  (`KismetSystemLibrary.K2_SetTimerDelegate` (delegate `TrySpawnActor`) (`self.SpawnTime`) true))

(event `TrySpawnActor`
  (if (< (`KismetArrayLibrary.Array_Length` (`self.Actors`)) (`self.MaxActors`))
    (`self.SpawnActor`)))

(event `SpawnActor`
  (bind _returnvalue (`|SpawnActorFromClass` (`self.ActorClass`) (`self.GetTransform`) "Undefined" "MultiplyWithRoot" null null))
  ;[1 1 1 0.33] Spawn default pawn controller
  (bind _aspawn (cast `Pawn` _returnvalue)
    (:`then`
      (`/Engine/EditorBlueprintResources/StandardMacros.IsValid` (`Pawn.GetController` _aspawn)
        (:`Is Valid`
          _)
        (:`Is Not Valid`
          (`Pawn.SpawnDefaultController` _aspawn))))
    (:`CastFailed`
      _))
  ;[1 1 1 0.33] Check if user don't want gravity
  (if (`self.No Gravity`)
    (bind _returnvalue_2 (`self.GetComponentByClass` _returnvalue "/Script/Engine.CharacterMovementComponent"))
    (`/Engine/EditorBlueprintResources/StandardMacros.IsValid` _returnvalue_2
      (:`Is Valid`
        (set `CharacterMovementComponent.GravityScale` 0.0 _returnvalue_2)
        (add `self.OnEndPlay` _returnvalue (delegate `OnActorEndPlay`) :!label _label)
        (`KismetArrayLibrary.Array_Add` (`self.Actors`) _returnvalue))
      (:`Is Not Valid`
        (`KismetSystemLibrary.PrintString` "Spider character movement is not valid" true true (struct :`R` 1.0 :`A` 1.0) 0.0)))
    (else
      (goto _label))))

(event `OnActorEndPlay` :!signature `self.OnEndPlay`
  (params (Actor :type "Actor Object Reference") (EndPlayReason :type "EEndPlayReason Enum" :default "Destroyed"))
  (`KismetArrayLibrary.Array_RemoveItem` (`self.Actors`) Actor))

(fn `UserConstructionScript`)