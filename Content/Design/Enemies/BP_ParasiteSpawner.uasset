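; Enemy spawner actor that creates parasite enemies at its own location and rotation.
; SpawnEnemy switches on the spawn info's enemy type, spawning BP_Parasite with its data asset and the spawner's cinematic mode, or printing an error for the unsupported Zero Enemy type.
; When auto-attack is set, it hands the player character to the new parasite's AI controller as its enemy.
; The event graph and construction script are empty.
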(fn `SpawnEnemy`
  (params (SpawnInfo :type "EnemySpawnerSpawnInfo Structure (by ref)"))
  (returns (ReturnValue :type "Actor Object Reference"))
  (bind (_returnvalue_location _returnvalue_rotation) (`KismetMathLibrary.BreakTransform` (`self.GetTransform`)))
  (switch `EEnemyType` SpawnInfo_EnemyType
    (:`ZeroEnemy`
      (`KismetSystemLibrary.PrintString` "ParasiteSpawner: Error: ZeroEnemy enemy type isn't supported!"))
    (:`Parasite`
      (bind _returnvalue (`|SpawnActorFromClass` "/Game/Design/Enemies/AI/Parasite/BP_Parasite.BP_Parasite_C" (`KismetMathLibrary.MakeTransform` _returnvalue_location _returnvalue_rotation) "AdjustIfPossibleButAlwaysSpawn" "MultiplyWithRoot" null SpawnInfo_ParasiteDataAsset (`self.CinematicMode`) null))
      (if SpawnInfo_bAutoAttackPlayer
        (`ParasiteAIController.SetEnemy` (cast `ParasiteAIController` (`Pawn.GetController` _returnvalue) :!pure true) (`GameplayStatics.GetPlayerCharacter` 0))
        (return _returnvalue)
        (else
          (return _returnvalue))))))

(fn `UserConstructionScript`)