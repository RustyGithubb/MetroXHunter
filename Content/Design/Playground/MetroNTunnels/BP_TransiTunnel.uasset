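; Modular metro tunnel piece whose boolean options cut the ceiling or either half, drop tracks or cables, and add left or right extensions.
; Construction Script and BeginPlay both apply the options through helpers that toggle visibility, collision and navigation relevance on mesh groups.
; The ceiling cut runs last in construction but first in BeginPlay, where enabled extensions re-show their side ceilings.
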(event `self.ReceiveBeginPlay`
  (if (`self.CutCeiling`)
    (`self.DisableCollisionAndVisibility` (`|MakeArray` (`self.SM_Ceiling`) (`self.SM_L_Ceiling`) (`self.SM_R_Ceiling`))))
  (if (`self.CutLeftHalf`)
    (`self.DisableCollisionAndVisibility` (`|MakeArray` (`self.SM_R_Cable`) (`self.SM_R_Wall`) (`self.SM_R_B_Wall`) (`self.SM_R_U_Wall_3`) (`self.SM_R_U_Wall_2`) (`self.SM_R_U_Wall_1`) (`self.SM_R_U_CornerWall`))))
  (if (`self.CutRightHalf`)
    (`self.DisableCollisionAndVisibility` (`|MakeArray` (`self.SM_L_B_Wall`) (`self.SM_L_Wall`) (`self.SM_L_Cable`) (`self.SM_L_U_Wall_2`) (`self.SM_L_U_Wall_3`) (`self.SM_L_U_Wall_1`) (`self.SM_L_U_CornerWall`))))
  (if (`self.WithoutTracks`)
    (`self.DisableCollisionAndVisibility` (`|MakeArray` (`self.SM_R_2Track`) (`self.SM_R_1Track`) (`self.SM_L_2Track`) (`self.SM_L_1Track`))))
  (if (`self.WithoutCables`)
    (`self.DisableCollisionAndVisibility` (`|MakeArray` (`self.SM_L_Cable`) (`self.SM_R_Cable`))))
  (if (`self.LeftExtension`)
    (`self.EnableCollisionAndVisibility` (`|MakeArray` (`self.SM_L_Ceiling`) (`self.SM_L_FloorPart`)))
    (else
      (`self.DisableCollisionAndVisibility` (`|MakeArray` (`self.SM_L_Ceiling`) (`self.SM_L_FloorPart`)))))
  (if (`self.RightExtension`)
    (`self.EnableCollisionAndVisibility` (`|MakeArray` (`self.SM_R_Ceiling`) (`self.SM_R_FloorPart`)))
    (else
      (`self.DisableCollisionAndVisibility` (`|MakeArray` (`self.SM_R_Ceiling`) (`self.SM_R_FloorPart`))))))

(fn `DisableCollisionAndVisibility`
  (params (`Static Meshes` :type "Array of StaticMeshComponent Object Reference") (Lights :type "Array of LightComponent Object Reference"))
  ;[1 0.5264 0.4766 0.33] DisableSM
  (for _array_element `Static Meshes`
    (`SceneComponent.SetHiddenInGame` _array_element true false)
    (`SceneComponent.SetVisibility` _array_element false false)
    (`PrimitiveComponent.SetCollisionEnabled` _array_element "NoCollision")
    (`UtilityLibrary.SetActorComponentCanEverAffectNavigation` _array_element))
  ;[1 0.8982 0.4238 0.33] DisableLights
  (for _array_element_2 Lights
    (`SceneComponent.SetHiddenInGame` _array_element_2 true false)
    (`SceneComponent.SetVisibility` _array_element_2 false false)
    (`UtilityLibrary.SetActorComponentCanEverAffectNavigation` _array_element_2))
  (return))

(fn `EnableCollisionAndVisibility`
  (params (`Static Meshes` :type "Array of StaticMeshComponent Object Reference") (Lights :type "Array of LightComponent Object Reference"))
  ;[1 0.5264 0.4766 0.33] DisableSM
  (for _array_element `Static Meshes`
    (`SceneComponent.SetHiddenInGame` _array_element false false)
    (`SceneComponent.SetVisibility` _array_element true false)
    (`PrimitiveComponent.SetCollisionEnabled` _array_element "QueryAndPhysics")
    (`UtilityLibrary.SetActorComponentCanEverAffectNavigation` _array_element true))
  ;[1 0.8982 0.4238 0.33] DisableLights
  (for _array_element_2 Lights
    (`SceneComponent.SetHiddenInGame` _array_element_2 false false)
    (`SceneComponent.SetVisibility` _array_element_2 true false)
    (`UtilityLibrary.SetActorComponentCanEverAffectNavigation` _array_element_2 true))
  (return))

(fn `UserConstructionScript`
  (locals (NewLocalVar :type "StaticMeshComponent Object Reference"))
  (if (`self.CutLeftHalf`)
    (`self.DisableCollisionAndVisibility` (`|MakeArray` (`self.SM_R_Cable`) (`self.SM_R_Wall`) (`self.SM_R_B_Wall`) (`self.SM_R_U_Wall_3`) (`self.SM_R_U_Wall_2`) (`self.SM_R_U_Wall_1`) (`self.SM_R_U_CornerWall`))))
  (if (`self.CutRightHalf`)
    (`self.DisableCollisionAndVisibility` (`|MakeArray` (`self.SM_L_B_Wall`) (`self.SM_L_Wall`) (`self.SM_L_Cable`) (`self.SM_L_U_Wall_2`) (`self.SM_L_U_Wall_3`) (`self.SM_L_U_Wall_1`) (`self.SM_L_U_CornerWall`))))
  (if (`self.WithoutTracks`)
    (`self.DisableCollisionAndVisibility` (`|MakeArray` (`self.SM_R_2Track`) (`self.SM_R_1Track`) (`self.SM_L_2Track`) (`self.SM_L_1Track`))))
  (if (`self.WithoutCables`)
    (`self.DisableCollisionAndVisibility` (`|MakeArray` (`self.SM_L_Cable`) (`self.SM_R_Cable`))))
  (if (`self.LeftExtension`)
    (`self.EnableCollisionAndVisibility` (`|MakeArray` (`self.SM_L_Ceiling`) (`self.SM_L_FloorPart`)))
    (else
      (`self.DisableCollisionAndVisibility` (`|MakeArray` (`self.SM_L_Ceiling`) (`self.SM_L_FloorPart`)))))
  (if (`self.RightExtension`)
    (`self.EnableCollisionAndVisibility` (`|MakeArray` (`self.SM_R_Ceiling`) (`self.SM_R_FloorPart`)))
    (else
      (`self.DisableCollisionAndVisibility` (`|MakeArray` (`self.SM_R_Ceiling`) (`self.SM_R_FloorPart`)))))
  (if (`self.CutCeiling`)
    (`self.DisableCollisionAndVisibility` (`|MakeArray` (`self.SM_Ceiling`) (`self.SM_L_Ceiling`) (`self.SM_R_Ceiling`)))))