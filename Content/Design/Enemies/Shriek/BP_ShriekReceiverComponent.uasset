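; Actor component that lets its owner receive enemy Shriek emissions and broadcast them after a simulated delay.
; The delay adds an optional sound travel time, from distance to the origin and shriek speed, to a random reaction time, with optional debug text.
; CanReceive defers to the owner when it implements BPI_ShriekReceiverExtra, and otherwise returns true.
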(event `ReceiveShriek`
  (params (EmissionContext :type "/Game/Design/Enemies/Shriek/F_ShriekEmissionContext Structure"))
  (bind (_totaldelay _heartime _reactiontime) (`self.ComputeShriekReceiveDelay` (`.Origin_5_775C6FF34AD5A1DD5792D89EE03C8C5E` (break `/Game/Design/Enemies/Shriek/F_ShriekEmissionContext` EmissionContext))))
  (if (`self.IsDrawDebugEnabled`)
    (`KismetSystemLibrary.DrawDebugString` (`Actor.K2_GetActorLocation` (`self.GetOwner`)) (`KismetTextLibrary.Conv_TextToString` (`|FormatText` "ShriekReceiver: Delayed by {TotalTime}s \n- HearTime: {HearTime}s \n- ReactionTime: {ReactionTime}s" _totaldelay _heartime _reactiontime)) null (struct :`G` 0.3 :`B` 1.0 :`A` 1.0) 5.0))
  (`KismetSystemLibrary.Delay` _totaldelay)
  (`self.OnShriekReceived` EmissionContext))

(fn `CanReceive`
  (params (Emitter :type "Actor Object Reference"))
  (returns (CanReceive :type Boolean))
  (bind _returnvalue (`self.GetOwner`))
  (if (`KismetSystemLibrary.DoesImplementInterface` _returnvalue "/Game/Design/Enemies/Shriek/BPI_ShriekReceiverExtra.BPI_ShriekReceiverExtra_C")
    (bind _canreceive (message `/Game/Design/Enemies/Shriek/BPI_ShriekReceiverExtra.CanReceiveShriek` _returnvalue Emitter))
    (return _canreceive)
    (else
      (return true))))

(fn `ComputeShriekReceiveDelay`
  (params (Origin :type "Vector Structure"))
  (returns (TotalDelay :type "Float (double-precision)") (HearTime :type "Float (double-precision)") (ReactionTime :type "Float (double-precision)"))
  (locals (ComputedHearTime :type "Float (double-precision)") (ComputedReactionTime :type "Float (double-precision)"))
  (bind _reactiontimerange (`self.ReactionTimeRange`))
  (bind _computedheartime (`local.ComputedHearTime`))
  (bind _computedreactiontime (`local.ComputedReactionTime`))
  (set `local.ComputedHearTime` (`KismetMathLibrary.SelectFloat` (/ (/ (`KismetMathLibrary.Vector_Distance` Origin (`Actor.K2_GetActorLocation` (`self.GetOwner`))) 100.0) (`self.ShriekSpeed`)) 0.0 (`self.IsAffectedByDistance`))) ; Why don't you want to compile when I name you 'HearTime'
  (set `local.ComputedReactionTime` (`KismetMathLibrary.RandomFloatInRange` (`.Value` (break `FloatRangeBound` (break `FloatRange` _reactiontimerange))) (`.Value` (break `FloatRangeBound` (`.UpperBound` (break `FloatRange` _reactiontimerange))))))
  (return (+ _computedheartime _computedreactiontime) _computedheartime _computedreactiontime))