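; Settings unit for the display (window) mode option among the graphics settings.
; On initialize, it loops over every EWindowMode value, filling an enum array and a parallel array of display texts converted from the enum names.
; On apply, it uses the selected index to look up the mode, sets it as the fullscreen mode on GameUserSettings and applies the settings.
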(event `self.OnApplySetting`
  (params (bInGame :type Boolean))
  (bind _returnvalue (`GameUserSettings.GetGameUserSettings`))
  (`GameUserSettings.SetFullscreenMode` _returnvalue (`|GetArrayItem` (`self.Enum Value`) (`self.IndexValue`)))
  (`GameUserSettings.ApplySettings` _returnvalue true))

(event `self.OnInitialize`
  (bind _enumvalue (foreach `EWindowMode` false)
    (:`LoopBody`
      (`KismetArrayLibrary.Array_Add` (`self.Enum Value`) _enumvalue)
      (`KismetArrayLibrary.Array_Add` (`self.EnumTexts`) (`KismetTextLibrary.Conv_StringToText` (`|GetEnumeratorNameAsString` _enumvalue))))))