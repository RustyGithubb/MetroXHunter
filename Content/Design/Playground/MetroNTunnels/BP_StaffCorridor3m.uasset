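; Modular 3 m staff corridor piece for the metro tunnels, with toggles for floor, ceiling, walls, inter-walls and two neon lights.
; Construction script and BeginPlay both apply the toggles, enabling visibility, collision and navigation on wanted parts and destroying unwanted components outright.
; Construction script also drives rect light intensity and neon dynamic materials from shared intensity and color.
; The right rect light's color is hardcoded black, unlike the left.
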(event `self.ReceiveBeginPlay`
  ;[1 1 1 0.33] Floor&Ceiling
  (if (`self.Floor`)
    (`self.EnableCollisionAndVisibility` (`|MakeArray` (`self.SM_Floor_3x3x0_5`)))
    (else
      (`self.DisableCollisionAndVisibility` (`|MakeArray` (`self.SM_Floor_3x3x0_5`)))))
  (if (`self.Ceiling`)
    (`self.EnableCollisionAndVisibility` (`|MakeArray` (`self.SM_Ceiling_3x3x0_5`)))
    (else
      (`self.DisableCollisionAndVisibility` (`|MakeArray` (`self.SM_Ceiling_3x3x0_5`)))))
  (if (`self.TopWall`)
    (`self.EnableCollisionAndVisibility` (`|MakeArray` (`self.SM_T_Wall_3x0_5x4`)))
    (else
      (`self.DisableCollisionAndVisibility` (`|MakeArray` (`self.SM_T_Wall_3x0_5x4`)))))
  (if (`self.BottomWall`)
    (`self.EnableCollisionAndVisibility` (`|MakeArray` (`self.SM_B_Wall_3x0_5x4`)))
    (else
      (`self.DisableCollisionAndVisibility` (`|MakeArray` (`self.SM_B_Wall_3x0_5x4`)))))
  (if (`self.LeftWall`)
    (`self.EnableCollisionAndVisibility` (`|MakeArray` (`self.SM_L_Wall_3x0_5x4`)))
    (else
      (`self.DisableCollisionAndVisibility` (`|MakeArray` (`self.SM_L_Wall_3x0_5x4`)))))
  (if (`self.RightWall`)
    (`self.EnableCollisionAndVisibility` (`|MakeArray` (`self.SM_R_Wall_3x0_5x4`)))
    (else
      (`self.DisableCollisionAndVisibility` (`|MakeArray` (`self.SM_R_Wall_3x0_5x4`)))))
  (if (`self.BottomLeftInterWall`)
    (`self.EnableCollisionAndVisibility` (`|MakeArray` (`self.SM_B_L_Inter_Wall_6x4`)))
    (else
      (`self.DisableCollisionAndVisibility` (`|MakeArray` (`self.SM_B_L_Inter_Wall_6x4`)))))
  (if (`self.BottomRightInterWall`)
    (`self.EnableCollisionAndVisibility` (`|MakeArray` (`self.SM_B_R_Inter_Wall_6x4`)))
    (else
      (`self.DisableCollisionAndVisibility` (`|MakeArray` (`self.SM_B_R_Inter_Wall_6x4`)))))
  (if (`self.TopLeftInterWall`)
    (`self.EnableCollisionAndVisibility` (`|MakeArray` (`self.SM_T_L_Inter_Wall_6x4`)))
    (else
      (`self.DisableCollisionAndVisibility` (`|MakeArray` (`self.SM_T_L_Inter_Wall_6x4`)))))
  (if (`self.TopRightInterWall`)
    (`self.EnableCollisionAndVisibility` (`|MakeArray` (`self.SM_T_R_Inter_Wall_6x4`)))
    (else
      (`self.DisableCollisionAndVisibility` (`|MakeArray` (`self.SM_T_R_Inter_Wall_6x4`)))))
  (if (`self.Left Light`)
    (`self.EnableCollisionAndVisibility` (`|MakeArray` (`self.SM_L_Neon`)) (`|MakeArray` (`self.L_RectLight`) :!type "LightComponent Object Reference"))
    (else
      (`self.DisableCollisionAndVisibility` (`|MakeArray` (`self.SM_L_Neon`)) (`|MakeArray` (`self.L_RectLight`) :!type "LightComponent Object Reference"))))
  (if (`self.Right Light`)
    (`self.EnableCollisionAndVisibility` (`|MakeArray` (`self.SM_R_Neon`)) (`|MakeArray` (`self.R_RectLight`) :!type "LightComponent Object Reference"))
    (else
      (`self.DisableCollisionAndVisibility` (`|MakeArray` (`self.SM_R_Neon`)) (`|MakeArray` (`self.R_RectLight`) :!type "LightComponent Object Reference")))))

(fn `DisableCollisionAndVisibility`
  (params (`Static Meshes` :type "Array of StaticMeshComponent Object Reference") (Lights :type "Array of LightComponent Object Reference"))
  ;[1 0.5264 0.4766 0.33] DisableSM
  (for _array_element `Static Meshes`
    (`/Engine/EditorBlueprintResources/StandardMacros.IsValid` _array_element
      (:`Is Valid`
        (`ActorComponent.K2_DestroyComponent` _array_element))))
  ;[1 0.8982 0.4238 0.33] DisableLights
  (for _array_element_2 Lights
    (`/Engine/EditorBlueprintResources/StandardMacros.IsValid` _array_element_2
      (:`Is Valid`
        (`ActorComponent.K2_DestroyComponent` _array_element_2))))
  (return))

(fn `EnableCollisionAndVisibility`
  (params (`Static Meshes` :type "Array of StaticMeshComponent Object Reference") (Lights :type "Array of LightComponent Object Reference"))
  ;[1 0.5264 0.4766 0.33] EnableSM
  (for _array_element `Static Meshes`
    (`/Engine/EditorBlueprintResources/StandardMacros.IsValid` _array_element
      (:`Is Valid`
        (`SceneComponent.SetHiddenInGame` _array_element false false)
        (`SceneComponent.SetVisibility` _array_element true false)
        (`PrimitiveComponent.SetCollisionEnabled` _array_element "QueryAndPhysics")
        (`UtilityLibrary.SetActorComponentCanEverAffectNavigation` _array_element true))))
  ;[1 0.8982 0.4238 0.33] EnableLights
  (for _array_element_2 Lights
    (`/Engine/EditorBlueprintResources/StandardMacros.IsValid` _array_element_2
      (:`Is Valid`
        (`SceneComponent.SetHiddenInGame` _array_element_2 false false)
        (`SceneComponent.SetVisibility` _array_element_2 true false)
        (`UtilityLibrary.SetActorComponentCanEverAffectNavigation` _array_element_2 true))))
  (return))

(fn `UserConstructionScript`
  (bind _sm_l_neon (`self.SM_L_Neon`))
  (bind _colorlight (`self.ColorLight`))
  (bind _sm_r_neon (`self.SM_R_Neon`))
  ;[1 0.8982 0.4238 0.33] Set Light
  ;;[1 1 1 0.33] In Candelas
  (`LightComponent.SetIntensity` (`self.L_RectLight`) (`self.IntensityLight`))
  (`LightComponent.SetIntensity` (`self.R_RectLight`) (`self.IntensityLight`))
  (bind _returnvalue (`PrimitiveComponent.CreateDynamicMaterialInstance` _sm_l_neon 0 (`PrimitiveComponent.GetMaterial` _sm_l_neon 0) "None"))
  (`MaterialInstanceDynamic.SetScalarParameterValue` _returnvalue "Intensity" (`self.IntensityLight`))
  (`MaterialInstanceDynamic.SetVectorParameterValue` _returnvalue "Color" _colorlight)
  (`LightComponent.SetLightColor` (`self.L_RectLight`) _colorlight true)
  (bind _returnvalue_2 (`PrimitiveComponent.CreateDynamicMaterialInstance` _sm_r_neon 0 (`PrimitiveComponent.GetMaterial` _sm_r_neon 0) "None"))
  (`MaterialInstanceDynamic.SetScalarParameterValue` _returnvalue_2 "Intensity" (`self.IntensityLight`))
  (`MaterialInstanceDynamic.SetVectorParameterValue` _returnvalue_2 "Color" (`self.ColorLight`))
  (`LightComponent.SetLightColor` :`self` (`self.R_RectLight`))
  ;[1 1 1 0.33] Floor&Ceiling
  (if (`self.Floor`)
    (`self.EnableCollisionAndVisibility` (`|MakeArray` (`self.SM_Floor_3x3x0_5`)))
    (else
      (`self.DisableCollisionAndVisibility` (`|MakeArray` (`self.SM_Floor_3x3x0_5`)))))
  (if (`self.Ceiling`)
    (`self.EnableCollisionAndVisibility` (`|MakeArray` (`self.SM_Ceiling_3x3x0_5`)))
    (else
      (`self.DisableCollisionAndVisibility` (`|MakeArray` (`self.SM_Ceiling_3x3x0_5`)))))
  (if (`self.TopWall`)
    (`self.EnableCollisionAndVisibility` (`|MakeArray` (`self.SM_T_Wall_3x0_5x4`)))
    (else
      (`self.DisableCollisionAndVisibility` (`|MakeArray` (`self.SM_T_Wall_3x0_5x4`)))))
  (if (`self.BottomWall`)
    (`self.EnableCollisionAndVisibility` (`|MakeArray` (`self.SM_B_Wall_3x0_5x4`)))
    (else
      (`self.DisableCollisionAndVisibility` (`|MakeArray` (`self.SM_B_Wall_3x0_5x4`)))))
  (if (`self.LeftWall`)
    (`self.EnableCollisionAndVisibility` (`|MakeArray` (`self.SM_L_Wall_3x0_5x4`)))
    (else
      (`self.DisableCollisionAndVisibility` (`|MakeArray` (`self.SM_L_Wall_3x0_5x4`)))))
  (if (`self.RightWall`)
    (`self.EnableCollisionAndVisibility` (`|MakeArray` (`self.SM_R_Wall_3x0_5x4`)))
    (else
      (`self.DisableCollisionAndVisibility` (`|MakeArray` (`self.SM_R_Wall_3x0_5x4`)))))
  (if (`self.BottomLeftInterWall`)
    (`self.EnableCollisionAndVisibility` (`|MakeArray` (`self.SM_B_L_Inter_Wall_6x4`)))
    (else
      (`self.DisableCollisionAndVisibility` (`|MakeArray` (`self.SM_B_L_Inter_Wall_6x4`)))))
  (if (`self.BottomRightInterWall`)
    (`self.EnableCollisionAndVisibility` (`|MakeArray` (`self.SM_B_R_Inter_Wall_6x4`)))
    (else
      (`self.DisableCollisionAndVisibility` (`|MakeArray` (`self.SM_B_R_Inter_Wall_6x4`)))))
  (if (`self.TopLeftInterWall`)
    (`self.EnableCollisionAndVisibility` (`|MakeArray` (`self.SM_T_L_Inter_Wall_6x4`)))
    (else
      (`self.DisableCollisionAndVisibility` (`|MakeArray` (`self.SM_T_L_Inter_Wall_6x4`)))))
  (if (`self.TopRightInterWall`)
    (`self.EnableCollisionAndVisibility` (`|MakeArray` (`self.SM_T_R_Inter_Wall_6x4`)))
    (else
      (`self.DisableCollisionAndVisibility` (`|MakeArray` (`self.SM_T_R_Inter_Wall_6x4`)))))
  (if (`self.Left Light`)
    (`self.EnableCollisionAndVisibility` (`|MakeArray` (`self.SM_L_Neon`)) (`|MakeArray` (`self.L_RectLight`) :!type "LightComponent Object Reference"))
    (else
      (`self.DisableCollisionAndVisibility` (`|MakeArray` (`self.SM_L_Neon`)) (`|MakeArray` (`self.L_RectLight`) :!type "LightComponent Object Reference"))))
  (if (`self.Right Light`)
    (`self.EnableCollisionAndVisibility` (`|MakeArray` (`self.SM_R_Neon`)) (`|MakeArray` (`self.R_RectLight`) :!type "LightComponent Object Reference"))
    (else
      (`self.DisableCollisionAndVisibility` (`|MakeArray` (`self.SM_R_Neon`)) (`|MakeArray` (`self.R_RectLight`) :!type "LightComponent Object Reference")))))