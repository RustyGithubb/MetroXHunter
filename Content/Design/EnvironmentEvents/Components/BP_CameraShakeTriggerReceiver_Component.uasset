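; Trigger receiver component for environment events that plays a world camera shake when its component-specific event fires.
; PlayOnPlayer centres the shake on player 0's pawn; otherwise it uses EpicenterIfNotPlayer as a world position, with inner and outer radii passed through.
; A debug function draws a temporary box at the owner's location plus EpicenterIfNotPlayer, treating that value as an offset, unlike the shake itself.
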(fn `DisplayEpicenterLocationVisualizer`
  (`KismetSystemLibrary.FlushPersistentDebugLines`)
  (`KismetSystemLibrary.DrawDebugBox` (+ (`Actor.K2_GetActorLocation` (`self.GetOwner`)) (`self.Epicenter if not Player`)) (5.0 5.0 5.0) (struct :`R` 1.0 :`B` 1.0 :`A` 1.0) (struct) 10.0 5.0))

(fn `OnPlayComponentSpecificEvent`
  (params (FromBoxEnter :type Boolean) (TriggerBox :type "Actor Object Reference"))
  (bind _inner_radius (`self.Inner Radius`))
  (bind _outer_radius (`self.Outer Radius`))
  (bind _shake (`self.Shake`))
  (if (`self.Play On Player`)
    (`GameplayStatics.PlayWorldCameraShake` _shake (`Actor.K2_GetActorLocation` (`GameplayStatics.GetPlayerPawn` 0)) _inner_radius _outer_radius)
    (else
      (`GameplayStatics.PlayWorldCameraShake` _shake (`self.Epicenter if not Player`) _inner_radius _outer_radius))))