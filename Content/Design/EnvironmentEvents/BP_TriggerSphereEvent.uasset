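; Placeable trigger sphere that fires level events when the player character (BP_Charles) enters or exits.
; At BeginPlay it caches receiver components from the linked actor, or itself if none is linked, printing a suppressible error if none exist.
; Overlaps notify those receivers only when required player flags match; one-time triggers destroy their components on exit.
; The construction script sizes the sphere and camera-aligned label, colouring the visualizer by one-time use.
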(event `self.ReceiveBeginPlay`
  (`self.GetReceiverComponent`)
  ;[1 1 1 0.33] Should Show Ingame? (for debug purposes probably)
  (`SceneComponent.SetHiddenInGame` (`self.DONT_MOVE_TriggerSphere`) (not (`self.ShowIngame`)) false)
  (`SceneComponent.SetHiddenInGame` (`self.TextRender`) (not (`self.ShowIngame`)) false)
  (`SceneComponent.SetHiddenInGame` (`self.VisualizerSphere`) (not (`self.ShowIngame`)) false)
  ;[1 1 1 0.33] Cache Player FlagComponent if we need to check flags
  (if (`BlueprintMapLibrary.Map_IsNotEmpty` (`self.NecessaryFlags`))
    (set `self.CharacterFlagComponent` (`self.GetComponentByClass` (`GameplayStatics.GetPlayerPawn` 0) "/Game/Design/EnvironmentEvents/BP_EventFlagsComponent.BP_EventFlagsComponent_C"))))

(event `self.DONT_MOVE_TriggerSphere.OnComponentBeginOverlap`
  (params (OverlappedComponent :type "PrimitiveComponent Object Reference") (OtherActor :type "Actor Object Reference") (OtherComp :type "PrimitiveComponent Object Reference") (OtherBodyIndex :type Integer) (bFromSweep :type Boolean) (SweepResult :type "HitResult Structure (by ref)"))
  ;[0.2889 0.3106 1 0.33] Is the actor that entered really our Main Character?
  ; The TriggerBox is set to only Overlap Pawns, but Enemies are probably gonna be pawns too
  (if (`/Game/Design/Libraries/BPL_GeneralUtilities.Is Object Of Class` OtherActor "/Game/Developers/corentinpaya/Collections/BP_Charles.BP_Charles_C")
    (bind _everythingright (`self.AreFlagsCorrect`))
    (if _everythingright
      (for _array_element (`self.ComponentsToCall`)
        (`/Game/Design/EnvironmentEvents/Components/BP_TriggerEventReceiver_Component.OnTriggerBoxEnter` _array_element self)))))

(event `self.DONT_MOVE_TriggerSphere.OnComponentEndOverlap`
  (params (OverlappedComponent :type "PrimitiveComponent Object Reference") (OtherActor :type "Actor Object Reference") (OtherComp :type "PrimitiveComponent Object Reference") (OtherBodyIndex :type Integer))
  ;[0.2889 0.3106 1 0.33] Is the actor that entered really our Main Character?
  ; The TriggerBox is set to only Overlap Pawns, but Enemies are probably gonna be pawns too
  (if (`/Game/Design/Libraries/BPL_GeneralUtilities.Is Object Of Class` OtherActor "/Game/Developers/corentinpaya/Collections/BP_Charles.BP_Charles_C")
    (bind _everythingright (`self.AreFlagsCorrect`))
    (if _everythingright
      (for _array_element (`self.ComponentsToCall`)
        (`/Game/Design/EnvironmentEvents/Components/BP_TriggerEventReceiver_Component.OnTriggerBoxExit` _array_element self))
      ;[1 0.4063 0.3165 0.33] Should Destroy after One-Time Use?
      (if (`self.OneTimeUse`)
        (`ActorComponent.K2_DestroyComponent` (`self.DONT_MOVE_TriggerSphere`))
        (`ActorComponent.K2_DestroyComponent` (`self.TextRender`))
        (`ActorComponent.K2_DestroyComponent` (`self.VisualizerSphere`))))))

(fn `AreFlagsCorrect`
  (returns (EverythingRight :type Boolean))
  (locals (Keys :type "Array of GameplayTag Structure") (Values :type "Array of Boolean") (isRight :type Boolean))
  (`self.CharacterFlagComponent`
    (:`then`
      (`|ExecutionSequence`
        (:`then_0`
          ;[1 1 1 0.33] Caching
          (bind _keys (`BlueprintMapLibrary.Map_Keys` (`self.NecessaryFlags`)))
          (set `local.Keys` _keys)
          (bind _values (`BlueprintMapLibrary.Map_Values` (`self.NecessaryFlags`)))
          (set `local.Values` _values)
          (set `local.isRight` true))
        (:`then_1`
          (for (_array_element _array_index) (`local.Keys`)
            (if (not (== (`/Game/Design/EnvironmentEvents/BP_EventFlagsComponent.GetFlagValue` (`self.CharacterFlagComponent`) _array_element) (`|GetArrayItem` (`local.Values`) _array_index)))
              (set `local.isRight` false)
              (break)))
          (return (`local.isRight`)))))
    (:`else`
      ;[1 1 1 0.33] No flags to check?
      ; Good to go!
      (return true))))

(fn `GetReceiverComponent`
  ;[0.04963 0.5881 1 0.33] Is this Box connected to an external Actor that stores the Components?
  (bind _linkedreceiveractor (`self.LinkedReceiverActor`)
    (:`then`
      ;[1 0.9531 0.4163 0.33] Does this linked Actor have Components?
      (`/Engine/EditorBlueprintResources/StandardMacros.IsValid` (`self.GetComponentByClass` _linkedreceiveractor "/Game/Design/EnvironmentEvents/Components/BP_TriggerEventReceiver_Component.BP_TriggerEventReceiver_Component_C")
        (:`Is Valid`
          ;[1 0.4331 0.6261 0.33] If yes save all Components
          (set `self.ComponentsToCall` (`self.K2_GetComponentsByClass` (`self.LinkedReceiverActor`) "/Game/Design/EnvironmentEvents/Components/BP_TriggerEventReceiver_Component.BP_TriggerEventReceiver_Component_C")))
        (:`Is Not Valid`
          ;[0.4676 1 0.4728 0.33] Else Print Error
          (if (not (`self.DontPrintError`)) :!label _label
            (`KismetSystemLibrary.PrintText` (`|FormatText` "TriggerSphereEvent with name {name} doesn't possess any Trigger Receiver Component itself; and isn't linked to an Actor possessing one. \nTo prevent this error, check the \"Don't Print Error\" on the TriggerBox" (`KismetSystemLibrary.GetDisplayName` self)) true true (struct :`R` 1.0 :`A` 1.0) 5000.0)))))
    (:`else`
      ;[0.5071 0.3153 1 0.33] Or are components stored on this Trigger?
      (bind _output_get (set `self.ComponentsToCall` (`self.K2_GetComponentsByClass` "/Game/Design/EnvironmentEvents/Components/BP_TriggerEventReceiver_Component.BP_TriggerEventReceiver_Component_C")))
      (if (not (`KismetArrayLibrary.Array_IsNotEmpty` _output_get))
        (goto _label)))))

(fn `UserConstructionScript`
  (bind (_spheresizehandle_x _spheresizehandle_y _spheresizehandle_z) (`KismetMathLibrary.BreakVector` (`self.SphereSizeHandle`)))
  (`self.TextMaterial`
    (:`then`
      _)
    (:`else`
      (bind _returnvalue (`PrimitiveComponent.CreateDynamicMaterialInstance` (`self.TextRender`) 0 "/Game/Art/0_Materials/Debug/M_CameraAlignedText.M_CameraAlignedText" "None"))
      (set `self.TextMaterial` _returnvalue)))
  ;[0 0 0 0.33] Set the correct size for the Trigger Box, the "OneTimeUse" visualizer box, and the Text inside (so it doesn't get too long)
  (`SceneComponent.K2_SetRelativeLocation` (`self.DONT_MOVE_TriggerSphere`) (0.0 0.0 0.0) false false)
  (`SphereComponent.SetSphereRadius` (`self.DONT_MOVE_TriggerSphere`) (`KismetMathLibrary.VSize` (`self.SphereSizeHandle`)) false)
  (`SceneComponent.SetRelativeScale3D` (`self.VisualizerSphere`) (`KismetMathLibrary.Conv_DoubleToVector` (* (`KismetMathLibrary.VSize` (`self.SphereSizeHandle`)) 0.02)))
  (`TextRenderComponent.SetWorldSize` (`self.TextRender`) (* (`KismetMathLibrary.FMax` (`KismetMathLibrary.FMax` (`KismetMathLibrary.Abs` _spheresizehandle_x) (`KismetMathLibrary.Abs` _spheresizehandle_y)) (`KismetMathLibrary.Abs` _spheresizehandle_z)) 0.25 (`self.TextScaleMultiplier`)))
  ;[0 0 0 0.33] Red if the TriggerBox is one-time-use
  ; Blue otherwise
  (`PrimitiveComponent.SetMaterial` (`self.VisualizerSphere`) 0 (select `bool` (`self.OneTimeUse`) :`false` "/Game/Art/0_Materials/Debug/Instances/MI_TranslucentBlue.MI_TranslucentBlue" :`true` "/Game/Art/0_Materials/Debug/Instances/MI_TranslucentRed.MI_TranslucentRed" :!type "MaterialInterface Object Reference"))
  ;[0 0 0 0.33] Set a custom visible name.
  ; I could use the "FitTextToNumberOfCharacters" but with the camera-oriented text and many different sizes possible for the TriggerBox, the LD is better of making line breaks themselves...
  (`TextRenderComponent.K2_SetText` (`self.TextRender`) (`self.TriggerCustomName`))
  ;[0 0 0 0.33] TextColor & Emissive
  (`TextRenderComponent.SetTextRenderColor` (`self.TextRender`) (`KismetMathLibrary.Conv_LinearColorToColor` (`self.TextColor`)))
  (`MaterialInstanceDynamic.SetScalarParameterValue` (`self.TextMaterial`) "TextEmissive" (`self.TextEmissiveIntensity`)))