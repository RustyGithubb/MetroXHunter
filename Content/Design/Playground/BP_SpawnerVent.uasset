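; Vent spawner that releases enemy creatures, up to a maximum count, when it receives a shriek or optionally on a random repeating timer.
; It async-loads the enemy class on BeginPlay and spawns one pawn at a time, blocking further requests while it exits.
; A timeline moves the pawn along a spline, then gives it its default controller and frees the vent.
; The lid-closing timeline is unconnected, and creature pooling remains a TO-DO.
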(event `self.ReceiveBeginPlay`
  (set `self.isOpen` true)
  (`|ExecutionSequence`
    (:`then_0`
      ;[1 1 1 0.33] Load EnemyClass
      (bind _class (`|LoadAssetClass` (`self.EnemyClass`))
        (:`Completed`
          (bind _asactor (castclass `Actor` _class))
          (set `self.EnemyClassToSpawn` _asactor))))
    (:`then_1`
      (if (`self.bShouldSpawnByTime`)
        (`KismetSystemLibrary.Delay` (`KismetMathLibrary.RandomFloatInRange` 7.0 12.0) :!label _label)
        (`self.RequestSpawnCreature`)
        (goto _label)))))

(event `CloseVent`
  (set `self.isOpen` true))

(event `PlayExitVentAnimation`
  (bind (_direction _normalizedspiderprogress) (`Timeline|SpiderExitVent` :!via `PlayFromStart`)
    (:`Update`
      (`self.K2_SetActorLocation` (`self.SpawnedEnemy`) (`SplineComponent.GetLocationAtTime` (`self.Spline`) _normalizedspiderprogress "World" false) false false))
    (:`Finished`
      (`Pawn.SpawnDefaultController` (`self.SpawnedEnemy`))
      (set `self.SpawnedEnemy` null) ; Reset spawned enemy reference
    )))

(event `self.BP_ShriekReceiverComponent.OnShriekReceived`
  (params (EmissionContext :type "/Game/Design/Enemies/Shriek/F_ShriekEmissionContext Structure"))
  (`self.RequestSpawnCreature`)
  (`KismetSystemLibrary.PrintString` "SpawnerVent: Requested by shriek"))

(fn `CanReceiveShriek`
  (params (Emitter :type "Actor Object Reference"))
  (returns (CanReceive :type Boolean))
  (return (not (`KismetSystemLibrary.IsValid` (`self.SpawnedEnemy`)))))

(fn `RequestSpawnCreature`
  (bind (_returnvalue_location _returnvalue_rotation) (`KismetMathLibrary.BreakTransform` (`SceneComponent.K2_GetComponentToWorld` (`self.SpawnPoint`))))
  (if (or (== (`self.SpawnedCreatures`) (`self.MaxSpawnedCreatures`)) (`KismetSystemLibrary.IsValid` (`self.SpawnedEnemy`)))
    (if (not (`self.isOpen`))
      (`self.CloseVent`))
    (else
      (`/Engine/EditorBlueprintResources/StandardMacros.IncrementInt` (`self.SpawnedCreatures`)
        (:`  `
          ;[0 0.03646 0.00325 0.33] TO-DO : Pool Creatures
          ; They are the big resource-intensive stuff in the game, so having a Pooling system sounds like a must, but this requires a way to turn them off and on, including AI, pathing, IK, etc.
          (bind _returnvalue (`|SpawnActorFromClass` (`self.EnemyClassToSpawn`) (`KismetMathLibrary.MakeTransform` _returnvalue_location _returnvalue_rotation) "AlwaysSpawn" "MultiplyWithRoot" null null))
          (bind _aspawn (cast `Pawn` _returnvalue))
          (set `self.SpawnedEnemy` _aspawn)
          (`self.PlayExitVentAnimation`))))))

(fn `UserConstructionScript`)