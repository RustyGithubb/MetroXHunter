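; Tunnel lamp prop with a spotlight and emissive mesh material that responds to flicker callbacks, optionally resting switched off.
; BeginPlay caches the original material and intensity; with ShouldOFF, it and AfterBereferenced black out the lamp.
; Flicker start applies neon and, for off lamps, feeds the cached intensity into LightData; stop restores the resting look.
; Each flicker update creates a dynamic material instance to scale emissive intensity.
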(event `self.ReceiveBeginPlay`
  (`KismetArrayLibrary.Array_Add` (`self.Materials`) (`PrimitiveComponent.GetMaterial` (`self.StaticMesh`) 1))
  (set `self.Original Light Intensity` (`LightComponentBase.Intensity` (`self.SpotLight`)))
  (if (`self.Should OFF`) :!label _label
    (`LightComponent.SetIntensity` (`self.SpotLight`) 0.0)
    (`PrimitiveComponent.SetMaterial` (`self.StaticMesh`) 1 "/Engine/EditorMeshes/ColorCalibrator/M_ClearCoatBlack.M_ClearCoatBlack")))

(event `After Be referenced`
  (goto _label))

(fn `OnFlickLightStart`
  (params (LightData :type "LightData Structure (by ref)"))
  (`PrimitiveComponent.SetMaterial` (`self.StaticMesh`) 1 "/Game/Art/0_Materials/Material_Instance/MI_Neon_White_lumen.MI_Neon_White_lumen")
  (if (`self.Should OFF`)
    (setmembers `LightData` :`StructRef` LightData :`OriginalLightIntensity` (`self.Original Light Intensity`))
    (return)))

(fn `OnFlickLightStop`
  (params (LightData :type "LightData Structure (by ref)"))
  (if (`self.Should OFF`)
    (`PrimitiveComponent.SetMaterial` (`self.StaticMesh`) 1 "/Engine/EditorMeshes/ColorCalibrator/M_ClearCoatBlack.M_ClearCoatBlack")
    (setmembers `LightData` :`StructRef` LightData :`OriginalLightIntensity` 0.0)
    (`LightComponent.SetIntensity` (`self.SpotLight`) 0.0)
    (return)
    (else
      (`PrimitiveComponent.SetMaterial` (`self.StaticMesh`) 1 (`|GetArrayItem` (`self.Materials`))))))

(fn `OnFlickLightTick`
  (params (DeltaTime :type "Float (single-precision)") (LightData :type "LightData Structure (by ref)"))
  (return))

(fn `OnFlickLightUpdate`
  (params (LightData :type "LightData Structure (by ref)") (IntensityScale :type "Float (single-precision)"))
  (bind _returnvalue (`PrimitiveComponent.CreateDynamicMaterialInstance` (`self.StaticMesh`) 1 "/Game/Art/0_Materials/Material_Instance/MI_Neon_White_lumen.MI_Neon_White_lumen" "None"))
  (`MaterialInstanceDynamic.SetScalarParameterValue` _returnvalue "Emissive Intensity" (* IntensityScale 25.0))
  (return))

(fn `RetrieveFlickableLights`
  (returns (ReturnValue :type "Array of LightComponent Object Reference"))
  (return (`|MakeArray` (`self.SpotLight`) :!type "LightComponent Object Reference")))

(fn `UserConstructionScript`)