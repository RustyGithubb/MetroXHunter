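; BP_CheatFunction_NoClip is a toggleable cheat that lets the player fly through the level without collision.
; OnCheat reads IsToggled to call Ghost or Walk on the CheatManager, raising player character MaxAcceleration tenfold while ghosting and setting it back to a hardcoded value afterwards.
; GetReferences caches the controlled pawn as BP_MainChara, though OnCheat fetches player character 0 directly instead.
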(event `self.OnCheat`
  (bind _cheatmanager (`self.CheatManager`))
  (bind _charactermovement (`Character.CharacterMovement` (`GameplayStatics.GetPlayerCharacter` 0)))
  (if (`self.bIsToggled`)
    (`CheatManager.Ghost` _cheatmanager)
    (set `CharacterMovementComponent.MaxAcceleration` 10000.0 _charactermovement)
    (else
      (`CheatManager.Walk` _cheatmanager)
      (set `CharacterMovementComponent.MaxAcceleration` 1000.0 _charactermovement))))

(fn `GetReferences`
  (bind _returnvalue (`Controller.K2_GetPawn` (`CheatManager.GetPlayerController` (`self.CheatManager`))))
  (`/Engine/EditorBlueprintResources/StandardMacros.IsValid` _returnvalue
    (:`Is Valid`
      (bind _asbp_main_chara (cast `/Game/Design/_GameManagement/BP_MainChara` _returnvalue))
      (set `self.As BP Main Chara` _asbp_main_chara))))