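; Sliding door puzzle element that toggles away from its preset open or closed state when UnlockGPE fires.
; The construction script places the door from DoorState, offsetting open doors by the mesh bounds along Z or X per DoorOpenType.
; A SmoothOpen timeline lerps it from its BeginPlay position to the opposite one.
; Helper names read inverted: Close functions slide to the open offset, Open functions back to closed.
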(event `self.ReceiveBeginPlay`
  (`parent.ReceiveBeginPlay`)
  (set `self.InitialDoorPosition` (`SceneComponent.RelativeLocation` (`self.Door`))))

(event `self.UnlockGPE`
  (params (DamageContext :type "/Game/Design/LifeSystem/Structs/F_DamageContext Structure"))
  (bind (_direction _smoothopen) (`Timeline|Timeline` :!via `PlayFromStart`)
    (:`Update`
      (set `self.Smooth Open` _smoothopen)
      (switch `/Game/Design/GPE/Doors/E_DoorState` (`self.DoorState`)
        (:`NewEnumerator1`
          (switch `/Game/Design/GPE/Doors/E_DoorOpenType` (`self.DoorOpenType`)
            (:`NewEnumerator0`
              (`self.CloseVerticaly` 1))
            (:`NewEnumerator3`
              (`self.CloseVerticaly` -1))
            (:`NewEnumerator1`
              (`self.CloseHorizontaly` -1))
            (:`NewEnumerator2`
              (`self.CloseHorizontaly` 1))))
        (:`NewEnumerator0`
          (switch `/Game/Design/GPE/Doors/E_DoorOpenType` (`self.DoorOpenType`)
            (:`NewEnumerator0`
              (`self.OpenVerticaly` :!label _label))
            (:`NewEnumerator3`
              (goto _label))
            (:`NewEnumerator1`
              (`self.OpenHorizontaly` :!label _label_2))
            (:`NewEnumerator2`
              (goto _label_2))))))))

(fn `CloseHorizontaly`
  (params (Multiplier :type Integer))
  (bind (_initialdoorposition_x _initialdoorposition_y _initialdoorposition_z) (`KismetMathLibrary.BreakVector` (`self.InitialDoorPosition`)))
  (bind _doorextent_x (`KismetMathLibrary.BreakVector` (`self.DoorExtent`)))
  (bind _returnvalue_x (`KismetMathLibrary.BreakVector` (+ (`self.DoorClosedPosition`) (`KismetMathLibrary.MakeVector` (* _doorextent_x (`local.Multiplier`))))))
  (`SceneComponent.K2_SetRelativeLocation` (`self.Door`) (`KismetMathLibrary.MakeVector` (`KismetMathLibrary.Lerp` _initialdoorposition_x _returnvalue_x (`self.Smooth Open`)) _initialdoorposition_y _initialdoorposition_z) false false))

(fn `CloseVerticaly`
  (params (Multiplier :type Integer))
  (bind (_doorextent_x _doorextent_y _doorextent_z) (`KismetMathLibrary.BreakVector` (`self.DoorExtent`)))
  (bind (_initialdoorposition_x _initialdoorposition_y _initialdoorposition_z) (`KismetMathLibrary.BreakVector` (`self.InitialDoorPosition`)))
  (bind (_returnvalue_x _returnvalue_y _returnvalue_z) (`KismetMathLibrary.BreakVector` (+ (`self.DoorClosedPosition`) (`KismetMathLibrary.MakeVector` 0.0 0.0 (* _doorextent_z (`local.Multiplier`))))))
  (`SceneComponent.K2_SetRelativeLocation` (`self.Door`) (`KismetMathLibrary.MakeVector` _initialdoorposition_x _initialdoorposition_y (`KismetMathLibrary.Lerp` _initialdoorposition_z _returnvalue_z (`self.Smooth Open`))) false false))

(fn `OpenHorizontaly`
  (bind _doorclosedposition_x (`KismetMathLibrary.BreakVector` (`self.DoorClosedPosition`)))
  (bind (_initialdoorposition_x _initialdoorposition_y _initialdoorposition_z) (`KismetMathLibrary.BreakVector` (`self.InitialDoorPosition`)))
  (`SceneComponent.K2_SetRelativeLocation` (`self.Door`) (`KismetMathLibrary.MakeVector` (`KismetMathLibrary.Lerp` _initialdoorposition_x _doorclosedposition_x (`self.Smooth Open`)) _initialdoorposition_y _initialdoorposition_z) false false))

(fn `OpenVerticaly`
  (bind (_doorclosedposition_x _doorclosedposition_y _doorclosedposition_z) (`KismetMathLibrary.BreakVector` (`self.DoorClosedPosition`)))
  (bind (_initialdoorposition_x _initialdoorposition_y _initialdoorposition_z) (`KismetMathLibrary.BreakVector` (`self.InitialDoorPosition`)))
  (`SceneComponent.K2_SetRelativeLocation` (`self.Door`) (`KismetMathLibrary.MakeVector` _initialdoorposition_x _initialdoorposition_y (`KismetMathLibrary.Lerp` _initialdoorposition_z _doorclosedposition_z (`self.Smooth Open`))) false false))

(fn `UserConstructionScript`
  (locals (DoorLocation :type "Vector Structure" :default (0.0 0.0 0.0)))
  (bind (_doorextent_x _doorextent_y _doorextent_z) (`KismetMathLibrary.BreakVector` (`self.DoorExtent`)))
  (bind (_doorextent_x_2 _doorextent_y_2 _doorextent_z_2) (`KismetMathLibrary.BreakVector` (`self.DoorExtent`)))
  (bind _doorextent_x_3 (`KismetMathLibrary.BreakVector` (`self.DoorExtent`)))
  (bind _doorextent_x_4 (`KismetMathLibrary.BreakVector` (`self.DoorExtent`)))
  (`parent.UserConstructionScript`)
  (set `self.DoorExtent` (* (`.BoxExtent` (`KismetSystemLibrary.GetComponentBounds` (`self.Door`))) 2.0))
  (switch `/Game/Design/GPE/Doors/E_DoorState` (`self.DoorState`)
    (:`NewEnumerator1`
      (set `local.DoorLocation` (`self.DoorClosedPosition`)))
    (:`NewEnumerator0`
      (switch `/Game/Design/GPE/Doors/E_DoorOpenType` (`self.DoorOpenType`)
        (:`NewEnumerator0`
          (set `local.DoorLocation` (+ (`self.DoorClosedPosition`) (`KismetMathLibrary.MakeVector` 0.0 0.0 _doorextent_z))))
        (:`NewEnumerator3`
          (set `local.DoorLocation` (+ (`self.DoorClosedPosition`) (`KismetMathLibrary.MakeVector` 0.0 0.0 (* _doorextent_z_2 -1.0)))))
        (:`NewEnumerator1`
          (set `local.DoorLocation` (+ (`self.DoorClosedPosition`) (`KismetMathLibrary.MakeVector` (* _doorextent_x_3 -1.0)))))
        (:`NewEnumerator2`
          (set `local.DoorLocation` (+ (`self.DoorClosedPosition`) (`KismetMathLibrary.MakeVector` _doorextent_x_4)))))))
  (`SceneComponent.K2_SetRelativeLocation` (`self.Door`) (`local.DoorLocation`) false false))