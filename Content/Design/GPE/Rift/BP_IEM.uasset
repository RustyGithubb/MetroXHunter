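; Placeable IEM device at a rift: the player spends a carried IEM to place it, then Shock damage can set it off.
; Interacting enables collision, swaps to the active mesh and starts cable and spark effects.
; Health death triggers a lightning curve to RiftLocation, an AOE effect and flickering of nearby lights through the game mode's LightManager.
; StopEmitter saves the consumed state and shuts down lightning, audio and the damage box.
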(event `self.ReceiveBeginPlay`
  (bind _returnvalue_location (`KismetMathLibrary.BreakTransform` (`SceneComponent.K2_GetComponentToWorld` (`self.LightningEffectPosition`))))
  (`PrimitiveComponent.SetCollisionEnabled` (`self.Sphere`) "NoCollision")
  (`PrimitiveComponent.SetCollisionEnabled` (`self.StaticMesh`) "NoCollision")
  (bind _returnvalue (`|SpawnActorFromClass` "/Lightnings/Blueprints/Examples/BP_LightningCurve.BP_LightningCurve_C" (`SceneComponent.K2_GetComponentToWorld` (`self.LightningEffectPosition`)) "Undefined" "MultiplyWithRoot" null null))
  (bind _output_get (set `self.LightningCurve` _returnvalue))
  (`LightningEmitter.DeactivateEmitter` _output_get)
  (setmembers `LightningAttachment` :`StructRef` (`LightningEmitter.SourceAttachment` _output_get) :`Location` _returnvalue_location))

(event `TriggerIEM`
  (`AudioParameterControllerInterface.SetTriggerParameter` (`self.Audio`) "ActivateStick")
  (bind _lightningcurve (`self.LightningCurve`)
    (:`then`
      (setmembers `LightningAttachment` :`StructRef` (`LightningEmitter.TargetAttachment` _lightningcurve) :`Location` (`self.RiftLocation`))
      (`LightningEmitter.ActivateEmitter` _lightningcurve true)
      (bind _asbp_metro_game_mode (cast `/Game/Design/_GameManagement/Core/BP_MetroGameMode` (`GameplayStatics.GetGameMode`)))
      ;[1 1 1 0.33] NEED TO LOOP
      (`LightManagerComponent.FlickerLightsInRadius` (`/Game/Design/_GameManagement/Core/BP_MetroGameMode.LightManager` _asbp_metro_game_mode) 2500.0 (`self.K2_GetActorLocation`) "/Game/Design/_GameManagement/Light/C_Flickering_Light.C_Flickering_Light")
      (set `self.bIsTriggered` true))
    (:`else`)))

(event `self.Health.OnDeath`
  (params (DamageContext :type "DamageContext Structure (by ref)"))
  (bind (_returnvalue_location _returnvalue_rotation) (`KismetMathLibrary.BreakTransform` (`SceneComponent.K2_GetComponentToWorld` (`self.LightningEffectPosition`))))
  (`self.TriggerIEM`)
  (bind _asbp_sparks (cast `/Game/Art/VFX/GPE/Lightnings/BP_Sparks` (`ChildActorComponent.ChildActor` (`self.VFX_Activation`))))
  (set `/Game/Art/VFX/GPE/Lightnings/BP_Sparks.BurstEnable` true _asbp_sparks)
  (`/Game/Art/VFX/GPE/Lightnings/BP_Sparks.EnableBurst` _asbp_sparks)
  (bind _returnvalue (`NiagaraFunctionLibrary.SpawnSystemAtLocation` "/Game/Art/VFX/NS_Electrics/NS_Lightning_IEM_Zone.NS_Lightning_IEM_Zone" _returnvalue_location _returnvalue_rotation))
  (set `self.LightningAOE` _returnvalue))

(event `self.InteractableComponent.OnInteract`
  (bind (_returnvalue_location _returnvalue_rotation) (`KismetMathLibrary.BreakTransform` (`SceneComponent.K2_GetComponentToWorld` (`self.LightningEffectPosition`))))
  (`AudioComponent.Play` (`self.Audio`) 0.0)
  ;[1 0 0.01285 0.33] BOUH CAST NOT GOOD
  (bind _asbp_charles (cast `/Game/Developers/corentinpaya/Collections/BP_Charles` (`GameplayStatics.GetPlayerPawn` 0)))
  (`/Game/Developers/corentinpaya/Collections/BP_Charles.RemoveIEM` _asbp_charles)
  (set `self.bIsPlaced` true)
  (`PrimitiveComponent.SetCollisionEnabled` (`self.Sphere`) "QueryAndPhysics")
  (`PrimitiveComponent.SetCollisionEnabled` (`self.StaticMesh`) "QueryAndPhysics")
  (`StaticMeshComponent.SetStaticMesh` (`self.StaticMesh`) "/Game/Art/0_Mesh/GPE/IEM/SM_IEM_Active.SM_IEM_Active")
  (bind _returnvalue (`NiagaraFunctionLibrary.SpawnSystemAtLocation` "/Game/Art/VFX/NS_Electrics/NS_Lightning_Cable.NS_Lightning_Cable" _returnvalue_location _returnvalue_rotation))
  (set `self.LightningCable` _returnvalue)
  (`self.RemoveInteractionComponent`)
  (bind _asbp_sparks (cast `/Game/Art/VFX/GPE/Lightnings/BP_Sparks` (`ChildActorComponent.ChildActor` (`self.VFX_Activation`))))
  (set `/Game/Art/VFX/GPE/Lightnings/BP_Sparks.BurstEnable` true _asbp_sparks)
  (`/Game/Art/VFX/GPE/Lightnings/BP_Sparks.EnableBurst` _asbp_sparks))

(event `self.ConsumeInteraction`
  (`PrimitiveComponent.SetCollisionEnabled` (`self.Sphere`) "QueryAndPhysics")
  (`StaticMeshComponent.SetStaticMesh` (`self.StaticMesh`) "/Game/Art/0_Mesh/GPE/IEM/SM_IEM_Active.SM_IEM_Active")
  (`self.RemoveInteractionComponent`))

(event `self.InnerCollision.OnComponentBeginOverlap`
  (params (OverlappedComponent :type "PrimitiveComponent Object Reference") (OtherActor :type "Actor Object Reference") (OtherComp :type "PrimitiveComponent Object Reference") (OtherBodyIndex :type Integer) (bFromSweep :type Boolean) (SweepResult :type "HitResult Structure (by ref)"))
  (if (not (`self.bIsPlaced`))
    (`StaticMeshComponent.SetStaticMesh` (`self.StaticMesh`) "/Game/Art/0_Mesh/GPE/IEM/SM_IEM_Inactive.SM_IEM_Inactive")))

(event `self.InnerCollision.OnComponentEndOverlap`
  (params (OverlappedComponent :type "PrimitiveComponent Object Reference") (OtherActor :type "Actor Object Reference") (OtherComp :type "PrimitiveComponent Object Reference") (OtherBodyIndex :type Integer))
  (if (not (`self.bIsPlaced`))
    (`StaticMeshComponent.SetStaticMesh` (`self.StaticMesh`) "/Game/Art/0_Mesh/GPE/IEM/SM_IEM_InactiveFarAway.SM_IEM_InactiveFarAway")))

(fn `CanCallTakeDamage`
  (params (DamageContext :type "DamageContext Structure (by ref)"))
  (returns (ReturnValue :type Boolean))
  (return true))

(fn `IsShownAsDamageableToPlayer`
  (params (DamageType :type "EDamageType Enum" :default "Generic") (HitResult :type "HitResult Structure (by ref)"))
  (returns (ReturnValue :type Boolean))
  (return (and (`|EnumEquality` DamageType "Shock") (`self.bCanTakeDamage`) (not (`self.bIsTriggered`)))))

(fn `StopEmitter`
  (bind _saveddata (`SaveLoadComponent.SavedData` (`self.SaveComponent`)))
  (bind _value (`StructUtilsFunctionLibrary.GetInstancedStructValue` _saveddata)
    (:`Valid`
      (bind _structout (setmembers `InteractableSavedData` :`StructRef` _value :`bIsConsummed` true))
      (`StructUtilsFunctionLibrary.SetInstancedStructValue` _saveddata _structout)
      (bind _lightningcurve (`self.LightningCurve`)
        (:`then`
          (`LightningEmitter.DeactivateEmitter` _lightningcurve)
          (bind _damagebox (`self.DamageBox`)
            (:`then`
              (`self.K2_DestroyActor` _damagebox))
            (:`else`
              _))
          (`NiagaraComponent.SetVariableFloat` (`self.LightningCable`) "Lightning Spawn Rate" 0.0)
          (`NiagaraComponent.SetVariableFloat` (`self.LightningAOE`) "Lightning Spawn Rate" 0.0)
          (`NiagaraComponent.SetVariableFloat` (`self.LightningCable`) "Sparks Spawn Rate" 0.0)
          (`ActorComponent.K2_DestroyComponent` (`self.VFX_Activation`))
          (`AudioParameterControllerInterface.SetTriggerParameter` (`self.Audio`) "Stop"))
        (:`else`)))))

(fn `TakeDamage`
  (params (DamageContext :type "DamageContext Structure (by ref)"))
  (returns (ReturnValue :type Boolean))
  (return (and (`|EnumEquality` (`.DamageType` (break `DamageContext` DamageContext)) "Shock") (`self.bCanTakeDamage`) (not (`self.bIsTriggered`)))))

(fn `UserConstructionScript`)