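; BP_SodaCan is a temporary soda can interactable that removes itself after a random lifetime.
; On BeginPlay it picks a lifespan within LifetimeRange and stores the Cylinder mesh's starting scale.
; During the final second, Tick multiplies that scale by the remaining lifespan, so the can shrinks smoothly before the engine destroys it.
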(event `self.ReceiveBeginPlay`
  (bind _lifetimerange (`self.LifetimeRange`))
  (`self.SetLifeSpan` (`KismetMathLibrary.RandomFloatInRange` (`.Value` (break `FloatRangeBound` (break `FloatRange` _lifetimerange))) (`.Value` (break `FloatRangeBound` (`.UpperBound` (break `FloatRange` _lifetimerange))))))
  (set `self.StartingScale` (`SceneComponent.RelativeScale3D` (`self.Cylinder`))))

(event `self.ReceiveTick`
  (params (DeltaSeconds :type "Float (single-precision)"))
  ;[1 1 1 0.33] if in the last second, get smaller before destroying
  (if (<= (`self.GetLifeSpan`) 1.0)
    (`SceneComponent.SetRelativeScale3D` (`self.Cylinder`) (* (`self.StartingScale`) (`self.GetLifeSpan`)))))

(fn `UserConstructionScript`)