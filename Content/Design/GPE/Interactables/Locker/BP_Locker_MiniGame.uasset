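; Interactable locker with a timed, joystick-driven skill check that swings the door open on success.
; Tick feeds rotation input to a WBP_LockerSkillCheck widget and runs the countdown display, while interaction presses start the check or get judged by the widget with haptic feedback.
; Timeout shocks and damages the player, then locks the game until a reset delay ends.
; A data asset supplies time limit, sounds and widget tuning.
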(event `self.ShowSkillCheckWidget`
  ;[1 1 1 0.33] Create and Add to viewport Skill Check Widget
  (bind _returnvalue (`|CreateWidget` "/Game/Design/Widgets/Interactions/WBP_LockerSkillCheck.WBP_LockerSkillCheck_C" (`GameplayStatics.GetPlayerController` 0)))
  (bind _output_get (set `self.SkillCheckWidget` _returnvalue))
  (`UserWidget.AddToViewport` _output_get 0)
  (`self.SetWidgetMembers`)
  (`/Game/Design/Widgets/Interactions/WBP_LockerSkillCheck.InitializeSkillCheck` _output_get))

(event `self.ReceiveTick`
  (params (DeltaSeconds :type "Float (single-precision)"))
  (bind _returnvalue (`GameplayStatics.GetPlayerCharacter` 0))
  ;[1 1 1 0.33] Update Skill Check Inputs
  (if (`self.bIsSkillCheckActive`)
    (`/Game/Design/Widgets/Interactions/WBP_LockerSkillCheck.UpdateJoystickVisualizer` (`self.SkillCheckWidget`) (* (`|GetInputActionValue`) (1.0 -1.0)))
    ;[1 1 1 0.33] Update Timer
    (bind _return (`/Game/Design/Libraries/BPL_GeneralUtilities.Decrease Value Float` (`self.CurrentTimer`) DeltaSeconds))
    (`|ExecutionSequence`
      (:`then_0`
        (if (<= _return 0.0)
          ;[1 1 1 0.33] Fail locker skill check
          (`self.EndSkillCheck` false)
          (set `self.CurrentTimer` 0.0)
          (`ActorComponent.Activate` (`self.Niagara`) false)
          (`KismetSystemLibrary.Delay` 0.2)
          (`self.RemoveSkillCheckWidget`)
          (`HealthComponent.TakeDamage` (`self.GetComponentByClass` _returnvalue "/Script/MetroXHunter.HealthComponent") (make `DamageContext` null 25 "Shock" self self))
          (`ElectrocutableComponent.Electrocute` (`self.GetComponentByClass` _returnvalue "/Script/MetroXHunter.ElectrocutableComponent") 1.0)
          (`KismetSystemLibrary.K2_ClearAndInvalidateTimerHandle` (`self.TimerHanlder_Tick`))
          (`self.ResetSkillCheck`)))
      (:`then_1`
        (`TextRenderComponent.K2_SetText` (`self.TextRender`) (`KismetTextLibrary.Conv_DoubleToText` (`self.CurrentTimer`) "HalfToEven" false true 1 1 1 1))))))

(event `self.RemoveSkillCheckWidget`
  ;[1 1 1 0.33] Remove Widget
  (`Widget.RemoveFromParent` (`self.SkillCheckWidget`)))

(event `self.OnSkillCheckAttempt`
  (bind _skillcheckwidget (`self.SkillCheckWidget`))
  ;[1 1 1 0.33] OnSkillCheckAttempt
  (if (`self.bIsSkillCheckActive`)
    (bind _caninteract (`/Game/Design/Widgets/Interactions/WBP_LockerSkillCheck.CanInteract` _skillcheckwidget))
    (if _caninteract
      (bind (_isfreefrominteraction _issequencefailed) (`/Game/Design/Widgets/Interactions/WBP_LockerSkillCheck.Receive Interaction Press` _skillcheckwidget))
      (`|ExecutionSequence`
        (:`then_0`
          (if _isfreefrominteraction
            (set `self.bIsGameEnded` false)
            (set `self.bIsSkillCheckActive` false)
            (`KismetSystemLibrary.Delay` 0.2)
            (`self.RemoveSkillCheckWidget`)
            (`self.OpenDoor`)
            (`KismetSystemLibrary.K2_ClearAndInvalidateTimerHandle` (`self.TimerHanlder_Tick`))
            (`self.EndSkillCheck` true)))
        (:`then_1`
          (`self.PlayHaptic` _issequencefailed))))
    (else
      (`self.StartSkillCheck`))))

(event `PlayHaptic`
  (params (IsSequenceFailed :type Boolean))
  (bind _returnvalue (`GameplayStatics.GetPlayerController` 0))
  ;[1 1 1 0.33] Haptic effect
  (if IsSequenceFailed
    (`PlayerController.PlayDynamicForceFeedback` _returnvalue 1.0 (`LockerData.PressCooldownPenalty` (`self.LockerDataAsset`)) true true true true)
    (else
      (`PlayerController.PlayDynamicForceFeedback` _returnvalue 0.1 0.1 true true true true))))

(event `OpenDoor`
  ;[1 1 1 0.33] Open Door
  (bind (_direction _doorrotations) (`Timeline|Timeline` :!via `PlayFromStart`)
    (:`Update`
      (`SceneComponent.K2_SetRelativeRotation` (`self.Door`) (`KismetMathLibrary.MakeRotator` 0.0 0.0 _doorrotations) false false))))

(event `self.StartSkillCheck`
  (if (not (`self.bIsGameEnded`))
    (set `self.bIsSkillCheckActive` true)
    (`/Game/Design/Widgets/Interactions/WBP_LockerSkillCheck.HideTutorialHUD` (`self.SkillCheckWidget`))
    (bind _returnvalue (`KismetSystemLibrary.K2_SetTimerDelegate` (`|CreateDelegate` :!event `TriggerSoundTick`) 1.0 true true))
    (set `self.TimerHanlder_Tick` _returnvalue)
    (`self.TriggerSoundTick`)))

(event `self.ResetSkillCheck`
  (set `self.bIsSkillCheckActive` false)
  (set `self.bIsGameEnded` true)
  (`KismetSystemLibrary.Delay` (`self.ResetTime`))
  (set `self.bIsGameEnded` false)
  (`self.InitialiazeTimer`))

(event `self.ConsumeInteraction`
  (`parent.ConsumeInteraction`)
  (`self.OpenDoor`))

(fn `InitialiazeTimer`
  (bind _timelimit (`LockerData.TimeLimit` (`self.LockerDataAsset`)))
  (set `self.CurrentTimer` _timelimit)
  (`TextRenderComponent.K2_SetText` (`self.TextRender`) (`KismetTextLibrary.Conv_DoubleToText` _timelimit "HalfToEven" false true 1 2 1 1)))

(fn `SetWidgetMembers`
  (bind _skillcheckwidget (`self.SkillCheckWidget`))
  (bind _lockerdataasset (`self.LockerDataAsset`))
  (bind _lockerdataasset_2 (`self.LockerDataAsset`))
  (set `/Game/Design/Widgets/Interactions/WBP_LockerSkillCheck.Sound_CorrectPress` (`LockerData.CorrectPressSound` _lockerdataasset_2) _skillcheckwidget)
  (set `/Game/Design/Widgets/Interactions/WBP_LockerSkillCheck.Sound_SequenceFailed` (`LockerData.SequenceFailedSound` _lockerdataasset_2) _skillcheckwidget)
  (set `/Game/Design/Widgets/Interactions/WBP_LockerSkillCheck.LineThickness` (`LockerData.LineThickness` _lockerdataasset) _skillcheckwidget)
  (set `/Game/Design/Widgets/Interactions/WBP_LockerSkillCheck.LineSmoothing` (`LockerData.LineSharpness` _lockerdataasset) _skillcheckwidget)
  (set `/Game/Design/Widgets/Interactions/WBP_LockerSkillCheck.TextureSize` (`LockerData.TextureSize` _lockerdataasset) _skillcheckwidget)
  (set `/Game/Design/Widgets/Interactions/WBP_LockerSkillCheck.PressCooldown` (`LockerData.PressCooldown` _lockerdataasset) _skillcheckwidget)
  (set `/Game/Design/Widgets/Interactions/WBP_LockerSkillCheck.SlerpSpeed` (`LockerData.JoystickSlerpSpeed` _lockerdataasset) _skillcheckwidget))

(fn `TriggerSoundTick`
  (`GameplayStatics.PlaySoundAtLocation` (`LockerData.TickSound` (`self.LockerDataAsset`)) (`SceneComponent.K2_GetComponentLocation` (`self.Screen`)) (struct) 1.0 1.0 0.0 (`self.Attenuation Settings`) null null null))

(fn `UserConstructionScript`
  (`self.InitialiazeTimer`))