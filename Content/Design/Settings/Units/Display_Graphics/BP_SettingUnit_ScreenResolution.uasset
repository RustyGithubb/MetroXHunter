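; Settings unit for the screen resolution option in the Display/Graphics settings.
; On initialize it applies the current resolution settings, gathers supported fullscreen resolutions, builds "WidthxHeight" option labels and defaults to the index matching the current resolution.
; On apply it sets the selected resolution through Game User Settings and applies the resolution settings.
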(event `self.OnApplySetting`
  (params (bInGame :type Boolean))
  (bind _returnvalue (`GameUserSettings.GetGameUserSettings`))
  (`GameUserSettings.SetScreenResolution` _returnvalue (`|GetArrayItem` (`self.Resolutions`) (`self.IndexValue`)))
  (`GameUserSettings.ApplyResolutionSettings` _returnvalue false))

(event `self.OnInitialize`
  (bind _returnvalue (`GameUserSettings.GetGameUserSettings`))
  (`GameUserSettings.ApplyResolutionSettings` _returnvalue false)
  (bind _resolutions (`KismetSystemLibrary.GetSupportedFullscreenResolutions`))
  (bind _output_get (set `self.Resolutions` _resolutions))
  (for (_array_element _array_index) _output_get
    (if (`KismetMathLibrary.Equal_IntPointIntPoint` _array_element (`GameUserSettings.GetScreenResolution` _returnvalue))
      (set `self.DefaultIndexValue` _array_index))
    (bind (_x _y) (break `IntPoint` _array_element))
    (`KismetArrayLibrary.Array_Add` (`self.EnumTexts`) (`KismetTextLibrary.Conv_StringToText` (`KismetStringLibrary.Concat_StrStr` (`KismetStringLibrary.Conv_IntToString` _x) "x" (`KismetStringLibrary.Conv_IntToString` _y))))))