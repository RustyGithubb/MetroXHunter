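; Trigger receiver component that plays a cinematic level sequence when its trigger event fires.
; The OnPlayComponentSpecificEvent function starts the Target's sequence player, then calls MoveTo, ignoring the trigger box arguments.
; MoveTo waits for a delay derived from the sequence's end frame and frame rate numerator.
; It then teleports the first player's pawn to its current location with zeroed rotation.
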(event `MoveTo`
  (bind _returnvalue (`GameplayStatics.GetPlayerPawn` 0))
  (bind _sequenceplayer (`LevelSequenceActor.SequencePlayer` (`self.Target`)))
  (bind _returnvalue_numerator (`KismetMathLibrary.BreakFrameRate` (`MovieSceneSequencePlayer.GetFrameRate` _sequenceplayer)))
  (`KismetSystemLibrary.Delay` (`KismetMathLibrary.Conv_IntToDouble` (/ (break `FrameNumber` (break `QualifiedFrameTime` (`MovieSceneSequencePlayer.GetEndTime` _sequenceplayer))) _returnvalue_numerator)))
  (set `self.Save Loc` (`Actor.K2_GetActorLocation` _returnvalue))
  (`Actor.K2_TeleportTo` :`self` _returnvalue :`DestLocation` (`self.Save Loc`)))

(fn `OnPlayComponentSpecificEvent`
  (params (FromBoxEnter :type Boolean) (TriggerBox :type "Actor Object Reference"))
  (`MovieSceneSequencePlayer.Play` (`LevelSequenceActor.SequencePlayer` (`self.Target`)))
  (`self.MoveTo`))