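; Game HUD that hosts the main viewport widget, toggles its game canvas and forwards screen text indications to it.
; On BeginPlay with a controlled pawn it creates the viewport, initializing child widgets a tick later as a stopgap for init order.
; It creates the cheat menu on first show and restores game input on hide.
; DrawHUD forwards to a debug component, while helpers draw material-based circles and crosshairs, creating a new crosshair material instance per draw.
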(event `self.ReceiveDrawHUD`
  (params (SizeX :type Integer) (SizeY :type Integer))
  (`/AdvancedAimAssist/Blueprints/Components/AAA_DebugHUDComponent.ReceiveDrawHUD` (`self.AAA_DebugHUDComponent`) SizeX SizeY))

(event `self.ReceiveBeginPlay`
  ;[1 1 1 0.33] Check is Simulating in Editor
  (`/Engine/EditorBlueprintResources/StandardMacros.IsValid` (`Controller.K2_GetPawn` (`self.PlayerOwner`))
    (:`Is Valid`
      (bind _returnvalue (`|CreateWidget` "/Game/Design/Widgets/WBP_Viewport.WBP_Viewport_C"))
      (bind _output_get (set `self.Viewport` _returnvalue))
      (`UserWidget.AddToViewport` _output_get 0)
      ;[0.2812 0.04834 0.1037] Please, change this at some point to only initialize the HUD when the rest is initialized; not just a random Delay...
      (`KismetSystemLibrary.DelayUntilNextTick`)
      (`/Game/Design/Widgets/WBP_Viewport.InitializeChildrenWidgets` (`self.Viewport`)))))

(event `self.SetUIMode`
  (params (bShouldHideUI :type Boolean))
  (`Widget.SetVisibility` (`/Game/Design/Widgets/WBP_Viewport.GameCanvas` (`self.Viewport`)) (select `bool` bShouldHideUI :`false` "Visible" :`true` "Hidden" :!type "ESlateVisibility Enum")))

(fn `DrawCircle`
  (params (Material :type "MaterialInterface Object Reference") (Radius :type "Float (double-precision)"))
  (bind _returnvalue (* Radius 2.0))
  (bind (_returnvalue_x _returnvalue_y) (`KismetMathLibrary.BreakVector2D` (- (/ (`self.HUDViewportSize`) (2.0 2.0)) (`KismetMathLibrary.MakeVector2D` Radius Radius))))
  (`self.DrawMaterialSimple` Material _returnvalue_x _returnvalue_y _returnvalue _returnvalue))

(fn `DrawCross`
  (params (ScreenLocation :type "Vector2D Structure") (InText :type String) (InColor :type "LinearColor Structure") (InSize :type "Float (double-precision)"))
  (bind (_returnvalue_x _returnvalue_y) (`KismetMathLibrary.BreakVector2D` (- ScreenLocation (0.0 0.0))))
  (bind _insize (`local.InSize`))
  (bind _returnvalue (/ (`local.InSize`) 2.0))
  (bind (_returnvalue_x_2 _returnvalue_y_2) (`KismetMathLibrary.BreakVector2D` (- (`local.ScreenLocation`) (`KismetMathLibrary.MakeVector2D` _returnvalue _returnvalue))))
  (`self.DrawText` (`local.InText`) (`local.InColor`) _returnvalue_x _returnvalue_y null 1.5)
  (bind _returnvalue_2 (`KismetMaterialLibrary.CreateDynamicMaterialInstance` "/AdvancedAimAssist/Debug/M_DebugCrossHair.M_DebugCrossHair"))
  (set `self.CrossHairMI` _returnvalue_2)
  (`|ExecutionSequence`
    (:`then_0`
      (`MaterialInstanceDynamic.SetVectorParameterValue` (`self.CrossHairMI`) "Color" (`local.InColor`)))
    (:`then_1`
      (`MaterialInstanceDynamic.SetScalarParameterValue` (`self.CrossHairMI`) "TextureSize" (`local.InSize`)))
    (:`then_2`
      (`MaterialInstanceDynamic.SetScalarParameterValue` (`self.CrossHairMI`) "LineSmoothingSize" (`self.CrossHairSmoothing`)))
    (:`then_3`
      (`MaterialInstanceDynamic.SetScalarParameterValue` (`self.CrossHairMI`) "LineWidth" (`self.CrossHairLineWidth`))
      (`self.DrawMaterialSimple` (`self.CrossHairMI`) _returnvalue_x_2 _returnvalue_y_2 _insize _insize))))

(fn `InitializeCircles`
  (params (InRadiuses :type "Array of Float (double-precision)"))
  (locals (MaterialInstance :type "MaterialInstanceDynamic Object Reference") (Colors :type "Array of LinearColor Structure") (CurrentColor :type "LinearColor Structure"))
  (set `self.Radiuses` InRadiuses)
  (`KismetArrayLibrary.Array_Clear` (`self.CirclesMI`))
  (for (_array_element _array_index) (`local.Colors`)
    (bind _returnvalue (`KismetMaterialLibrary.CreateDynamicMaterialInstance` "/AdvancedAimAssist/Debug/M_DebugCircle.M_DebugCircle"))
    (set `local.MaterialInstance` _returnvalue)
    (`|ExecutionSequence`
      (:`then_0`
        (`MaterialInstanceDynamic.SetVectorParameterValue` (`local.MaterialInstance`) "Color" _array_element))
      (:`then_1`
        (`MaterialInstanceDynamic.SetScalarParameterValue` (`local.MaterialInstance`) "TextureSize" (* (`|GetArrayItem` (`self.Radiuses`) _array_index) 2.0)))
      (:`then_2`
        (`MaterialInstanceDynamic.SetScalarParameterValue` (`local.MaterialInstance`) "LineThickness" (`self.CircleThickness`)))
      (:`then_3`
        (`MaterialInstanceDynamic.SetScalarParameterValue` (`local.MaterialInstance`) "LineSmoothingSize" (`self.CircleSmoothing`))
        (`KismetArrayLibrary.Array_AddUnique` (`self.CirclesMI`) (`local.MaterialInstance`))))))

(fn `ReceiveEvent`
  (params (CalledTag :type "GameplayTag Structure") (CallingObject :type "Object Object Reference (by ref)"))
  (returns (Return :type Boolean))
  (return false))

(fn `ShowHideCheatMenuVisibility`
  (params (CheatManager :type "MetroCheatManager Object Reference") (PlayerController :type "PlayerController Object Reference") (bNewVisibility :type Boolean) (bShouldToggle :type Boolean))
  (returns (ReturnValue :type Boolean))
  (bind _playercontroller (`local.PlayerController`))
  (`/Engine/EditorBlueprintResources/StandardMacros.IsValid` CheatManager
    (:`Is Valid`
      (if bShouldToggle
        (set `self.isCheatMenuVisible` (not (`self.isCheatMenuVisible`)))
        (else
          (set `self.isCheatMenuVisible` bNewVisibility)))
      (if (`self.isCheatMenuVisible`)
        (bind _cheatmenu (`self.CheatMenu`)
          (:`then`
            (`/Game/Design/Widgets/CheatMenu/WBP_CheatMenu.ShowCheatMenu` _cheatmenu))
          (:`else`
            ;[0.4427 0.1807 0.3046 0.33] Push (create & set focus) CheatMenu
            (bind _returnvalue (`CommonActivatableWidgetContainerBase.BP_AddWidget` (`/Game/Design/Widgets/WBP_Viewport.CheatMenuSlot` (`self.Viewport`)) "/Game/Design/Widgets/CheatMenu/WBP_CheatMenu.WBP_CheatMenu_C"))
            (bind _output_get (set `self.CheatMenu` _returnvalue))
            (`/Game/Design/Widgets/CheatMenu/WBP_CheatMenu.Populate Cheats` _output_get (`local.CheatManager`))))
        (return (`self.isCheatMenuVisible`))
        (else
          (bind _cheatmenu_2 (`self.CheatMenu`)
            (:`then`
              (`/Game/Design/Widgets/CheatMenu/WBP_CheatMenu.HideCheatMenu` _cheatmenu_2)
              (`WidgetBlueprintLibrary.SetInputMode_GameOnly` _playercontroller)
              (set `PlayerController.bShowMouseCursor` false _playercontroller)
              (return (`self.isCheatMenuVisible`)))
            (:`else`)))))))

(fn `ShowNewTextIndication`
  (params (TextToShow :type "Text (by ref)"))
  (`/Game/Design/Widgets/WBP_ScreenIndications.SetNewIndication` (`/Game/Design/Widgets/WBP_Viewport.WBP_ScreenIndications` (`self.Viewport`)) TextToShow)
  (return))

(fn `UserConstructionScript`)