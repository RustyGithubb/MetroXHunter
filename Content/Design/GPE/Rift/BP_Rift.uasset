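; Rift encounter actor that the player closes through linked IEMs and a parasite fight.
; Interacting with every IEM makes them vulnerable; triggering them all by damage starts scripted events and registers the rift as an attacker, with parasites launched at the player via SpawnEnemy.
; Once events finish and no attackers remain, a timed closing sequence plays VFX, audio and light flicker, fires trigger receivers, then saves its destruction so it stays gone on load.
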(event `self.ReceiveBeginPlay`
  (bind _saveload (`self.SaveLoad`))
  (`|ExecutionSequence`
    (:`then_0`
      ;[1 1 1 0.33] Force Load if the Actor is initialized to late on the level streaming
      (`KismetSystemLibrary.DelayUntilNextTick`)
      (if (not (`SaveLoadComponent.bIsDataLoaded` _saveload))
        (`SaveLoadComponent.Load` _saveload)))
    (:`then_1`
      (`AudioComponent.SetSound` (`self.Audio`) (`/Game/Sounds/DataAssets/BP_RiftSoundData.IdleLoopSound` (`self.SoundData`))))
    (:`then_2`
      ;[1 1 1 0.33] Get IEMs
      (set `self.MyTriggerComponents` (`self.K2_GetComponentsByClass` "/Game/Design/EnvironmentEvents/Components/BP_TriggerEventReceiver_Component.BP_TriggerEventReceiver_Component_C"))
      (for (_array_element _array_index) (`self.IEMs`)
        (`/Engine/EditorBlueprintResources/StandardMacros.IsValid` _array_element
          (:`Is Valid`
            (set `/Game/Design/GPE/Rift/BP_IEM.RiftLocation` (`SceneComponent.K2_GetComponentLocation` (`self.Niagara`)) _array_element)
            ;;[1 1 1 0.33] Bind to events
            (bind _interactablecomponent (`BaseInteractable.InteractableComponent` _array_element)
              (:`then`
                (add `InteractableComponent.OnInteract` _interactablecomponent (`|CreateDelegate` :!event `IncrementIEMsReadyCount`))
                (bind _health (`/Game/Design/GPE/Rift/BP_IEM.Health` _array_element)
                  (:`then`
                    (add `HealthComponent.OnDeath` _health (`|CreateDelegate` :!event `IncrementIEMsActiveCount`)))
                  (:`else`)))
              (:`else`)))
          (:`Is Not Valid`
            (`KismetSystemLibrary.PrintText` (`|FormatText` "Rift: Invalid IEM reference at index {Index}, please update!" _array_index) true true (struct :`R` 1.0 :`A` 1.0) 10.0)))))))

(event `IncrementIEMsReadyCount`
  (bind _returnvalue (`self.GetComponentByClass` (`GameplayStatics.GetPlayerPawn` 0) "/Game/Design/Language/BPAC_DialogueManager.BPAC_DialogueManager_C"))
  ;[1 1 1 0.33] INCREMENT IEMs READY COUNT
  (`/Engine/EditorBlueprintResources/StandardMacros.IncrementInt` (`self.ReadyIEMsCount`)
    (:`  `
      (if (>= (`self.ReadyIEMsCount`) (`KismetArrayLibrary.Array_Length` (`self.IEMs`)))
        (`self.UpdateIEMsVulnerability`)
        (if (`self.First Rift`)
          (`DialogueManagerComponent.SetDialogueNamespace` _returnvalue "Script_ShootEMP")
          (`DialogueManagerComponent.StartDialogue` _returnvalue))))))

(event `Make Camera Shake`
  ;[1 1 1 0.33 42] EFFECT DURING FIGHT
  (`CameraShakeSourceComponent.Start` (`self.CameraShakeSource`))
  (`LightManagerComponent.FlickerLightsInRadius` (`self.GetComponentByClass` (`GameplayStatics.GetGameMode`) "/Script/MetroXHunter.LightManagerComponent") 2000.0 (`self.K2_GetActorLocation`) "/Game/Design/_GameManagement/Light/C_Flickering_Light.C_Flickering_Light"))

(event `IncrementIEMsActiveCount`
  (params (DamageContext :type "DamageContext Structure (by ref)"))
  (bind _startscriptedeventmanager (`self.StartScriptedEventManager`))
  ;[1 1 1 0.33] INCREMENT IEMs ACTIVE COUNT
  ;;[1 1 1 0.33] Check for IEMs count
  (bind _result (`/Engine/EditorBlueprintResources/StandardMacros.IncrementInt` (`self.ActiveIEMsCount`))
    (:`  `
      (if (== _result (`KismetArrayLibrary.Array_Length` (`self.IEMs`)))
        (`ScriptedEventManager.RunScriptedEvents` _startscriptedeventmanager)
        (add `ScriptedEventManager.OnEventsFinished` _startscriptedeventmanager (delegate `OnEventsFinished_Event`))
        (set `CameraShakeSourceComponent.CameraShake` "/Game/Design/_GameManagement/3C/CameraShake/BPCS_WorldShake_Medium.BPCS_WorldShake_Medium_C" (`self.CameraShakeSource`))
        (`AITargetComponent.DeclareAttacker` (`self.GetComponentByClass` (`GameplayStatics.GetPlayerCharacter` 0) "/Script/MetroXHunter.AITargetComponent") (`self.AIAttacker`))
        (else
          ;[1 1 1 0.33 42] EFFECT DURING FIGHT
          (`/Engine/EditorBlueprintResources/StandardMacros.DoOnce` false
            (:`Completed`
              (`CameraShakeSourceComponent.Start` (`self.CameraShakeSource`))
              (bind _returnvalue (`KismetSystemLibrary.K2_SetTimerDelegate` (delegate `Make Camera Shake`) 3.0 true))
              (set `self.CameraSequencerTimerHandle` _returnvalue))))))))

(event `OnEventsFinished_Event`
  (params (Manager :type "ScriptedEventManager Object Reference"))
  ;[1 1 1 0.33] INCREMENT IEMs ACTIVE COUNT
  (if (not (`self.bIsSpawningEnemy`))
    (`self.RetireRiftFromAttackers`)
    (else
      (set `self.bWantToRetireRiftAtNextSpawn` true))))

(event `self.SaveLoad.OnLoadActor`
  ;[0 1 0.05748 0.33] ON LOAD
  (bind _value (`StructUtilsFunctionLibrary.GetInstancedStructValue` (`SaveLoadComponent.SavedData` (`self.SaveLoad`)))
    (:`Valid`
      (if (not (`.bShouldSpawn` (break `BaseSavedData` _value)))
        (`self.Call tag and set flag`)
        (`self.K2_DestroyActor`)))))

(event `OnAttackersUpdate_Event`
  (params (AITargetComponent :type "AITargetComponent Object Reference"))
  ;[1 1 1 0.33] Auto-Kill when Combat is finished
  (if (== (`AITargetComponent.GetAttackersCount` AITargetComponent) 0)
    (`self.CloseRift`)))

(event `CloseRift`
  ;[1 1 1 0.33] Close Rift
  ;;[1 1 1 0.33] Update Niagara
  (`NiagaraComponent.SetAsset` (`self.Niagara`) "/Game/Art/VFX/NS_Rift_Final/NS_Rift_V1_Closing.NS_Rift_V1_Closing" true)
  (`self.Call tag and set flag`)
  (`KismetSystemLibrary.K2_ClearAndInvalidateTimerHandle` (`self.CameraSequencerTimerHandle`))
  (`CameraAnimationCameraModifier.PlayCameraAnimation` :`self` (`CameraAnimationCameraModifier.GetCameraAnimationCameraModifierFromPlayerController` (`GameplayStatics.GetPlayerController` 0)) :`Sequence` "/Game/Design/_GameManagement/3C/CameraAnimation/Environemental/CS_FirstRift_Loop_Simple.CS_FirstRift_Loop_Simple")
  (`AudioComponent.SetSound` (`self.Audio`) (`/Game/Sounds/DataAssets/BP_RiftSoundData.CloseLoopSound` (`self.SoundData`)))
  (`|ExecutionSequence`
    (:`then_0`
      (`KismetSystemLibrary.Delay` 10.5)
      (for _array_element (`self.MyTriggerComponents`)
        (`/Game/Design/EnvironmentEvents/Components/BP_TriggerEventReceiver_Component.OnTriggerBoxEnter` _array_element self)
        (set `self.MaximumTriggerDelay` (`KismetMathLibrary.FMax` (`/Game/Design/EnvironmentEvents/Components/BP_TriggerEventReceiver_Component.DelayBeforeActivation` _array_element) (`self.MaximumTriggerDelay`))))
      (for _array_element_2 (`self.IEMs`)
        (`/Game/Design/GPE/Rift/BP_IEM.StopEmitter` _array_element_2))
      (`KismetSystemLibrary.Delay` (`self.MaximumTriggerDelay`))
      (`self.SaveDeath`)
      (`self.K2_DestroyActor`))
    (:`then_1`
      ;;[0.03121 0 0.9948] CE JOUE A L'INSTANT DE L'EXPLOSION DE LA FAILLE
      (`KismetSystemLibrary.Delay` 9.0)
      (`LightManagerComponent.FlickerLightsInRadius` (`self.GetComponentByClass` (`GameplayStatics.GetGameMode`) "/Script/MetroXHunter.LightManagerComponent") 5000.0 (`self.K2_GetActorLocation`) "/Game/Design/_GameManagement/Light/C_Flickering_ShutDown6seconds.C_Flickering_ShutDown6seconds"))
    (:`then_2`
      ;;[1 1 1 0.33] CALL EVENT PROXY FOR IMMEDIATE ACTIONS
      (bind _riftcloseeventproxy (`self.RiftCloseEventProxy`)
        (:`then`
          (for _array_element_3 (`self.K2_GetComponentsByClass` _riftcloseeventproxy "/Game/Design/EnvironmentEvents/Components/BP_TriggerEventReceiver_Component.BP_TriggerEventReceiver_Component_C")
            (`/Game/Design/EnvironmentEvents/Components/BP_TriggerEventReceiver_Component.OnTriggerBoxEnter` _array_element_3 self)))
        (:`else`)))))

(event `RetireRiftFromAttackers`
  (bind _returnvalue (`self.GetComponentByClass` (`GameplayStatics.GetPlayerCharacter` 0) "/Script/MetroXHunter.AITargetComponent"))
  (`AITargetComponent.RetireAttacker` _returnvalue (`self.AIAttacker`))
  (if (== (`AITargetComponent.GetAttackersCount` _returnvalue) 0)
    (`self.CloseRift`)
    (else
      (add `AITargetComponent.OnAttackersUpdate` _returnvalue (`|CreateDelegate` :!event `OnAttackersUpdate_Event`)))))

(event `SpawnEnemies`
  (params (SpawnInfos :type "EnemySpawnerSpawnInfo Structure"))
  (bind (_bautoattackplayer _enemytype _zerodataasset _parasitedataasset) (break `EnemySpawnerSpawnInfo` SpawnInfos))
  (bind _niagara (`self.Niagara`))
  ;[1 0 0 0.33 32] SPAWN PARASITES
  (set `self.bIsSpawningEnemy` true)
  (`NiagaraFunctionLibrary.SpawnSystemAtLocation` "/Game/Art/VFX/NS_Distortion/NS_Distortion_SpawnParasite.NS_Distortion_SpawnParasite" (`self.K2_GetActorLocation`) (`self.K2_GetActorRotation`))
  (`FXSystemComponent.SetFloatParameter` _niagara "Center Attraction Force" 15000.0)
  (`KismetSystemLibrary.Delay` (`self.DelaySpawningVFX`))
  (`FXSystemComponent.SetFloatParameter` _niagara "Center Attraction Force" 800.0)
  (if (`|EnumEquality` _enemytype "Parasite")
    (bind _output_get (set `self.DirectionToPlayer` (`KismetMathLibrary.GetDirectionUnitVector` (`self.K2_GetActorLocation`) (`self.K2_GetActorLocation` (`GameplayStatics.GetPlayerCharacter` 0)))))
    (bind _returnvalue (`|SpawnActorFromClass` "/Game/Design/Enemies/AI/Parasite/BP_Parasite.BP_Parasite_C" (`KismetMathLibrary.MakeTransform` (+ (`self.K2_GetActorLocation`) (* _output_get (`self.ParasiteSpawnBackOffset`))) (`KismetMathLibrary.Conv_VectorToRotator` _output_get)) "Undefined" "MultiplyWithRoot" null _parasitedataasset "None" null))
    (`Character.LaunchCharacter` _returnvalue (* (`self.DirectionToPlayer`) (`self.ParasiteLaunchedForce`)) true false)
    (`ParasiteAIController.SetEnemy` (cast `ParasiteAIController` (`Pawn.GetController` _returnvalue) :!pure true) (`GameplayStatics.GetPlayerCharacter` 0))
    (set `self.bIsSpawningEnemy` false)
    (if (`self.bWantToRetireRiftAtNextSpawn`)
      (`self.RetireRiftFromAttackers`)
      (set `self.bWantToRetireRiftAtNextSpawn` false))
    (else
      (`KismetSystemLibrary.PrintText` (`|FormatText` "{ActorName}: Spawning {EnemyType} is not supported on this actor!" self (`|GetEnumeratorNameAsString` _enemytype)) true true (struct :`R` 1.0 :`A` 1.0) 10.0))))

(event `self.EffectBox.OnComponentBeginOverlap`
  (params (OverlappedComponent :type "PrimitiveComponent Object Reference") (OtherActor :type "Actor Object Reference") (OtherComp :type "PrimitiveComponent Object Reference") (OtherBodyIndex :type Integer) (bFromSweep :type Boolean) (SweepResult :type "HitResult Structure (by ref)"))
  ;[1 1 1 0.33 32] EFFECTS WHEN PLAYER STAYS IN THE BOX
  (`AudioModulationStatics.ActivateBusMix` "/Game/Sounds/Audio/SD/Modulation/ControlBusMix/CBM_Rift.CBM_Rift")
  (`AudioComponent.FadeIn` (`self.AudioRiftInside`) 3.0 1.0 0.5 "Linear"))

(event `self.EffectBox.OnComponentEndOverlap`
  (params (OverlappedComponent :type "PrimitiveComponent Object Reference") (OtherActor :type "Actor Object Reference") (OtherComp :type "PrimitiveComponent Object Reference") (OtherBodyIndex :type Integer))
  ;[1 1 1 0.33 32] EFFECTS WHEN PLAYER STAYS IN THE BOX
  (`AudioModulationStatics.DeactivateBusMix` "/Game/Sounds/Audio/SD/Modulation/ControlBusMix/CBM_Rift.CBM_Rift")
  (`AudioComponent.FadeOut` (`self.AudioRiftInside`) 1.5 0.0 "Linear"))

(fn `Call tag and set flag`
  (bind _tag_to_call_ending (`self.Tag to Call Ending`))
  (if (not (== (`self.Tag to Call Ending`) (struct)))
    (`/EventDispatcherHub/FunctionLibrary/BPL_EventDispatcherHub.Call Single Gameplay Event` _tag_to_call_ending self)
    (`/Game/Design/EnvironmentEvents/BP_EventFlagsComponent.SetFlagValue` (`self.GetComponentByClass` (`GameplayStatics.GetPlayerPawn` 0) "/Game/Design/EnvironmentEvents/BP_EventFlagsComponent.BP_EventFlagsComponent_C") _tag_to_call_ending true)))

(fn `SaveDeath`
  (bind _saveload (`self.SaveLoad`))
  (bind _saveddata (`SaveLoadComponent.SavedData` _saveload))
  (bind _value (`StructUtilsFunctionLibrary.GetInstancedStructValue` _saveddata)
    (:`Valid`
      (bind _structout (setmembers `BaseSavedData` :`StructRef` _value :`bShouldSpawn` false))
      (`StructUtilsFunctionLibrary.SetInstancedStructValue` _saveddata _structout)
      (`SaveLoadComponent.Save` _saveload))))

(fn `SpawnEnemy`
  (params (SpawnInfo :type "EnemySpawnerSpawnInfo Structure (by ref)"))
  (returns (ReturnValue :type "Actor Object Reference"))
  (locals (DirectionToPlayer :type "Vector Structure" :default (0.0 0.0 0.0)))
  (`self.SpawnEnemies` SpawnInfo)
  (return null))

(fn `UpdateIEMsVulnerability`
  (for _array_element (`self.IEMs`)
    (set `/Game/Design/GPE/Rift/BP_IEM.bCanTakeDamage` true _array_element)))

(fn `UserConstructionScript`)