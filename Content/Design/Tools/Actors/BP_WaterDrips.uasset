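; BP_WaterDrips is an actor that configures a Niagara water drip effect.
; A shared SetupNiagara function runs from both the construction script and BeginPlay, so the same setup applies in the editor and at runtime.
; It sets fixed system bounds from BoundMin and BoundMax, enables the WaterImpact emitter according to IsWater, and passes a texture to the system.
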(event `self.ReceiveBeginPlay`
  (`self.SetupNiagara`))

(fn `SetupNiagara`
  (bind _niagara (`self.Niagara`))
  (`NiagaraComponent.SetSystemFixedBounds` _niagara (`KismetMathLibrary.MakeBox` (`self.BoundMin`) (`self.BoundMax`)))
  (`FXSystemComponent.SetEmitterEnable` _niagara "WaterImpact" (`self.bIsWater`))
  (`NiagaraComponent.SetVariableTexture` _niagara "Texture" (`self.Texture`)))

(fn `UserConstructionScript`
  (`self.SetupNiagara`))