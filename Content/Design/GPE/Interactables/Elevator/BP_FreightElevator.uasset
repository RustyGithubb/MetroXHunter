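; One-use interactable freight elevator that dispenses a pickup based on the player's health and inventory.
; On interact, two chained placeholder timelines slide the Cube door along Y then Z, then SpawnItem runs and interaction is removed.
; SpawnItem gives a full syringe load at half health or below, otherwise tops up missing syringes, else spawns fixed ammo if not full, or nothing.
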(event `self.InteractableComponent.OnInteract`
  (bind _cube (`self.Cube`))
  (bind _cube_2 (`self.Cube`))
  (bind (_relativelocation_x _relativelocation_y _relativelocation_z) (`KismetMathLibrary.BreakVector` (`SceneComponent.RelativeLocation` _cube_2)))
  (bind (_relativelocation_x_2 _relativelocation_y_2) (`KismetMathLibrary.BreakVector` (`SceneComponent.RelativeLocation` _cube)))
  ;[1 1 1 0.33] PLACEHOLDER - Window Animation
  ;;[1 1 1 0.33] Y Translation
  (bind (_direction _newtrack_1) (`Timeline|DoorAnimation1` :!via `PlayFromStart`)
    (:`Update`
      (`SceneComponent.K2_SetRelativeLocation` _cube_2 (`KismetMathLibrary.MakeVector` _relativelocation_x (+ (* _newtrack_1 -4.0) -48.0) _relativelocation_z) false false))
    (:`Finished`
      ;;[1 1 1 0.33] Z Translation
      (bind (_direction_2 _newtrack_1_2) (`Timeline|DoorAnimation2` :!via `PlayFromStart`)
        (:`Update`
          (`SceneComponent.K2_SetRelativeLocation` _cube (`KismetMathLibrary.MakeVector` _relativelocation_x_2 _relativelocation_y_2 (* _newtrack_1_2 80.0)) false false))
        (:`Finished`
          (`self.SpawnItem`)
          (`self.RemoveInteractionComponent`))))))

(fn `SpawnItem`
  (bind _returnvalue (`GameplayStatics.GetPlayerCharacter` 0))
  (bind _returnvalue_2 (`self.GetComponentByClass` _returnvalue "/Script/MetroXHunter.HealthComponent"))
  (bind (_returnvalue_location _returnvalue_rotation) (`KismetMathLibrary.BreakTransform` (`SceneComponent.K2_GetComponentToWorld` (`self.ItemSpawnPoint`))))
  (bind _returnvalue_3 (`self.GetComponentByClass` _returnvalue "/Script/MetroXHunter.InventoryComponent"))
  (bind (_returnvalue_location_2 _returnvalue_rotation_2) (`KismetMathLibrary.BreakTransform` (`SceneComponent.K2_GetComponentToWorld` (`self.ItemSpawnPoint`))))
  (bind (_returnvalue_location_3 _returnvalue_rotation_3) (`KismetMathLibrary.BreakTransform` (`SceneComponent.K2_GetComponentToWorld` (`self.ItemSpawnPoint`))))
  (bind _inventorydataasset (`InventoryComponent.InventoryDataAsset` _returnvalue_3))
  (bind _maxsyringecapacity (`InventoryData.MaxSyringeCapacity` _inventorydataasset))
  (bind _returnvalue_4 (- _maxsyringecapacity (`InventoryComponent.CurrentSyringeAmount` _returnvalue_3)))
  ;[1 1 1 0.33] Check if LOW LIFE
  (if (> (/ (`HealthComponent.CurrentHealth` _returnvalue_2) (`HealthComponent.MaxHealth` _returnvalue_2)) 0.5)
    ;[1 1 1 0.33] Check if syringe not full
    (if (== _returnvalue_4 0)
      ;[1 1 1 0.33] Check if ammo not full
      (if (< (`InventoryComponent.CurrentAmmoAmount` _returnvalue_3) (`InventoryData.MaxAmmoAmountCapacity` _inventorydataasset))
        (bind _returnvalue_5 (`|SpawnActorFromClass` "/Game/Design/GPE/PickupLoot/BP_Ammo.BP_Ammo_C" (`KismetMathLibrary.MakeTransform` _returnvalue_location _returnvalue_rotation) "Undefined" "MultiplyWithRoot" null null))
        (set `BasePickUp.Amount` 30 _returnvalue_5))
      (else
        (bind _returnvalue_6 (`|SpawnActorFromClass` "/Game/Design/GPE/PickupLoot/BP_Syringe.BP_Syringe_C" (`KismetMathLibrary.MakeTransform` _returnvalue_location_3 _returnvalue_rotation_3) "Undefined" "MultiplyWithRoot" null null))
        (set `BasePickUp.Amount` _returnvalue_4 _returnvalue_6)))
    (else
      (bind _returnvalue_7 (`|SpawnActorFromClass` "/Game/Design/GPE/PickupLoot/BP_Syringe.BP_Syringe_C" (`KismetMathLibrary.MakeTransform` _returnvalue_location_2 _returnvalue_rotation_2) "Undefined" "MultiplyWithRoot" null null))
      (set `BasePickUp.Amount` _maxsyringecapacity _returnvalue_7))))

(fn `UserConstructionScript`)