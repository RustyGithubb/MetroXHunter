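; Trigger-event receiver component that switches an array of BP_SmartLight actors on or off, playing a switch sound at each light.
; Without SwitchWithTimer, a trigger event simply applies ShouldOFF to every light.
; In timer mode, box entry enables tick, where a FlipFlop blinks the lights as the tick interval shrinks toward roughly 0.3 seconds.
; Box exit stops the tick and applies a false ShouldOFF to all lights.
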(event `self.ReceiveTick`
  (params (DeltaSeconds :type "Float (single-precision)"))
  (if (`self.Switch with Timer`)
    (bind _isa (`/Engine/EditorBlueprintResources/StandardMacros.FlipFlop`)
      (:`A`
        (`self.Swith All Light` _isa))
      (:`B`
        (`self.Swith All Light` _isa)))
    (if (not (<= (`self.Tick Interval`) 0.3))
      (bind _output_get (set `self.Tick Interval` (- (`self.Tick Interval`) (/ (`self.Tick Interval`) 15.0) 0.01)))
      (`self.SetComponentTickInterval` _output_get))))

(fn `OnPlayComponentSpecificEvent`
  (params (FromBoxEnter :type Boolean) (TriggerBox :type "Actor Object Reference"))
  (if (`self.Switch with Timer`)
    (if FromBoxEnter
      (`self.SetComponentTickInterval` (`self.Tick Interval`))
      (`self.SetComponentTickEnabled` true)
      (else
        (`self.SetComponentTickEnabled` false)
        (`self.Swith All Light` false)))
    (else
      (`self.Swith All Light` (`self.Should OFF`)))))

(fn `Swith All Light`
  (params (`Should OFF` :type Boolean))
  (for _array_element (`self.Array of Actor`)
    (bind _asbp_smart_light (cast `/Game/Art/0_Mesh/GPE/BP_SmartLight` _array_element))
    (`/Game/Art/0_Mesh/GPE/BP_SmartLight.Actualise State Light` _asbp_smart_light `Should OFF`)
    (`GameplayStatics.PlaySoundAtLocation` "/Engine/VREditor/Sounds/UI/Flashlight_Switch.Flashlight_Switch" (`Actor.K2_GetActorLocation` _asbp_smart_light) (struct) 1.0 1.0 0.0 "/Game/Sounds/Attenuations/SA_Reverb.SA_Reverb" null null null)))