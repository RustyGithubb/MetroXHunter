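; BP_Blind is a blind in the MetroNTunnels playground that opens on the PlaytestOctober OpenBlind gameplay tag event.
; It binds to that event at BeginPlay, and ReceiveEvent calls OpenBlind, which instantly raises the mesh and plays a sound.
; The construction script previews the Open flag; the sound position derives from the mesh's relative location, not world.
; Helpers for toggling mesh and light visibility, collision and navigation are never called here.
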(event `self.ReceiveBeginPlay`
  (`/EventDispatcherHub/FunctionLibrary/BPL_EventDispatcherHub.Bind to Single Gameplay Event` (struct :`TagName` "event.Room.PlaytestOctober.OpenBlind") self))

(fn `DisableCollisionAndVisibility`
  (params (`Static Meshes` :type "Array of StaticMeshComponent Object Reference") (Lights :type "Array of LightComponent Object Reference"))
  ;[1 0.5264 0.4766 0.33] DisableSM
  (for _array_element `Static Meshes`
    (`SceneComponent.SetHiddenInGame` _array_element true false)
    (`SceneComponent.SetVisibility` _array_element false false)
    (`PrimitiveComponent.SetCollisionEnabled` _array_element "NoCollision")
    (`UtilityLibrary.SetActorComponentCanEverAffectNavigation` _array_element))
  ;[1 0.8982 0.4238 0.33] DisableLights
  (for _array_element_2 Lights
    (`SceneComponent.SetHiddenInGame` _array_element_2 true false)
    (`SceneComponent.SetVisibility` _array_element_2 false false)
    (`UtilityLibrary.SetActorComponentCanEverAffectNavigation` _array_element_2))
  (return))

(fn `EnableCollisionAndVisibility`
  (params (`Static Meshes` :type "Array of StaticMeshComponent Object Reference") (Lights :type "Array of LightComponent Object Reference"))
  ;[1 0.5264 0.4766 0.33] EnableSM
  (for _array_element `Static Meshes`
    (`SceneComponent.SetHiddenInGame` _array_element false false)
    (`SceneComponent.SetVisibility` _array_element true false)
    (`PrimitiveComponent.SetCollisionEnabled` _array_element "QueryAndPhysics")
    (`UtilityLibrary.SetActorComponentCanEverAffectNavigation` _array_element true))
  ;[1 0.8982 0.4238 0.33] EnableLights
  (for _array_element_2 Lights
    (`SceneComponent.SetHiddenInGame` _array_element_2 false false)
    (`SceneComponent.SetVisibility` _array_element_2 true false)
    (`UtilityLibrary.SetActorComponentCanEverAffectNavigation` _array_element_2 true))
  (return))

(fn `OpenBlind`
  (set `self.Open` true)
  (`SceneComponent.K2_SetRelativeLocation` (`self.Blind`) (0.0 0.0 425.0) false false)
  (`GameplayStatics.PlaySoundAtLocation` "/Game/Sounds/Audio/SFX/SFX_GPE/SFX_Blind/SC_BlindOpening.SC_BlindOpening" (+ (`SceneComponent.RelativeLocation` (`self.Blind`)) (200.0 0.0 500.0)) (struct) 1.0 1.0 0.0 null null null null))

(fn `ReceiveEvent`
  (params (CalledTag :type "GameplayTag Structure") (CallingObject :type "Object Object Reference (by ref)"))
  (returns (Return :type Boolean))
  (`|SwitchGameplayTag` CalledTag
    (:`event.Room.PlaytestOctober.OpenBlind`
      (`self.OpenBlind`)
      (return false))))

(fn `UserConstructionScript`
  (if (`self.Open`)
    (`SceneComponent.K2_SetRelativeLocation` (`self.Blind`) (0.0 0.0 425.0) false false)
    (else
      (`SceneComponent.K2_SetRelativeLocation` (`self.Blind`) (0.0 0.0 0.0) false false))))