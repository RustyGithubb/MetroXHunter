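; Settings unit that lets the game switch its language among the available localized cultures.
; On initialize it fills parallel culture and option-text lists with localized display names, defaulting to English in the editor and French otherwise.
; On apply it sets the culture at the selected index as current, without saving it to config.
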(event `self.OnInitialize`
  (bind _cultures (`self.Cultures`))
  (for _array_element (`KismetInternationalizationLibrary.GetLocalizedCultures` true)
    (`KismetArrayLibrary.Array_Add` _cultures _array_element)
    (`KismetArrayLibrary.Array_Add` (`self.EnumTexts`) (`KismetTextLibrary.Conv_StringToText` (`KismetInternationalizationLibrary.GetCultureDisplayName` _array_element))))
  (set `self.DefaultIndexValue` (`KismetArrayLibrary.Array_Find` _cultures (`KismetMathLibrary.SelectString` "en" "fr" (`UtilityLibrary.IsWithinEditor`)))))

(event `self.OnApplySetting`
  (params (bInGame :type Boolean))
  (`KismetInternationalizationLibrary.SetCurrentCulture` (`|GetArrayItem` (`self.Cultures`) (`self.IndexValue`))))