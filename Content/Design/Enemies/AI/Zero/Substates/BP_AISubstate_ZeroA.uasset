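; BP_AISubstate_ZeroA is an AI substate for the Zero enemy, apparently a timed placeholder step in its behavior.
; On entering, it prints a debug message naming the controlled pawn.
; Each tick it returns Next once the manager's substate time passes a fixed threshold and the pawn is not rushing, otherwise Stay.
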(event `self.OnSubstateEntered`
  (`parent.OnSubstateEntered`)
  (`KismetSystemLibrary.PrintText` (`|FormatText` "Substate A for {Enemy}" (`ZeroEnemyAIController.CustomPawn` (`self.AIController`)))))

(fn `TickSubstate`
  (params (DeltaTime :type "Float (single-precision)"))
  (returns (ReturnValue :type "EAISubstateSwitchOrder Enum"))
  (if (and (> (`AISubstateManagerComponent.GetSubstateTime` (`self.Manager`)) 5.0) (not (`ZeroEnemy.IsRushing` (`ZeroEnemyAIController.CustomPawn` (`self.AIController`)))))
    (return "Next")
    (else
      (return "Stay"))))