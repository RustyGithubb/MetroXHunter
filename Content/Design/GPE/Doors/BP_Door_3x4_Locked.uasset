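; Locked swing door that starts with interaction frozen until a tagged gameplay event plays its open sequence and unlocks it.
; Opening plays a sound, removes interaction, rotates the door on a timeline and saves the consumed, open state, which skips the unlock binding on later loads.
; A close event resets rotation and removes interaction.
; The construction script uses FlipRotation to set swing direction, mesh offset and arrow.
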(event `self.ReceiveBeginPlay`
  (bind (_relativerotation_roll _relativerotation_pitch _relativerotation_yaw) (`KismetMathLibrary.BreakRotator` (`SceneComponent.RelativeRotation` (`self.Door`))))
  (`KismetSystemLibrary.DelayUntilNextTick`)
  (set `self.StartYawRotation` _relativerotation_yaw)
  (`self.SetInteractionFreezed` true)
  (`/EventDispatcherHub/FunctionLibrary/BPL_EventDispatcherHub.Bind to Single Gameplay Event` (`self.Tag to Bind Close`) self)
  (bind _value (`StructUtilsFunctionLibrary.GetInstancedStructValue` (`SaveLoadComponent.SavedData` (`self.SaveComponent`)))
    (:`Valid`
      (if (not (`.bIsConsummed` (break `InteractableSavedData` _value)))
        (`/EventDispatcherHub/FunctionLibrary/BPL_EventDispatcherHub.Bind to Single Gameplay Event` (`self.Tag to bind Open`) self)))))

(event `self.SetDoorOpened`
  (params (bShouldOpen :type Boolean))
  (if bShouldOpen
    (`ActorSequenceComponent.StopSequence` (`self.Open Actor sequence`))
    (`GameplayStatics.PlaySoundAtLocation` "/Game/Sounds/Audio/SD/MetaSounds/MS_Sources/GPE/Doors/MS_Doors.MS_Doors" (`SceneComponent.K2_GetComponentLocation` (`self.AudioPos`)) (struct) 1.0 1.0 0.0 "/Game/Sounds/Audio/SD/Att/Att_30m.Att_30m" null null null)
    (`self.InteractableComponent`
      (:`then`
        (`self.SetInteractionFreezed` true)
        (`self.RemoveInteractionComponent`))
      (:`else`
        _))
    (bind _output_get (set `self.bIsOpened` true))
    (`self.SaveConsumeInteraction` _output_get)
    (bind (_direction _rotation) (`Timeline|OpenDoor` :!via `PlayFromStart`)
      (:`Update`
        (`SceneComponent.K2_SetRelativeRotation` (`self.Door`) (`KismetMathLibrary.MakeRotator` 0.0 0.0 (+ (* _rotation (`self.FinalRotation`)) (`self.StartYawRotation`))) false false)))))

(event `self.CloseDoorEditor`
  (`SceneComponent.K2_SetRelativeRotation` (`self.Door`) (`KismetMathLibrary.MakeRotator` 0.0) false false))

(fn `Close Grid`
  (`SceneComponent.K2_SetRelativeRotation` :`self` (`self.Door`))
  (`self.RemoveInteractionComponent`))

(fn `OpenGrid`
  (`ActorSequenceComponent.PlaySequence` (`self.Open Actor sequence`))
  (`self.SetInteractionFreezed` false)
  (set `self.bIsLocked` false))

(fn `ReceiveEvent`
  (params (CalledTag :type "GameplayTag Structure") (CallingObject :type "Object Object Reference (by ref)"))
  (returns (Return :type Boolean))
  (if (== CalledTag (`self.Tag to bind Open`))
    (`self.OpenGrid`)
    (return false)
    (elif (== CalledTag (`self.Tag to Bind Close`))
      (`self.Close Grid`)
      (return false))))

(fn `SaveConsumeInteraction`
  (params (`Should Start Open` :type Boolean))
  (bind _saveddata (`SaveLoadComponent.SavedData` (`self.SaveComponent`)))
  (bind _value (`StructUtilsFunctionLibrary.GetInstancedStructValue` _saveddata)
    (:`Valid`
      (bind _structout (setmembers `InteractableSavedData` :`StructRef` _value :`bIsConsummed` true :`bShouldStartOpen` `Should Start Open`))
      (`StructUtilsFunctionLibrary.SetInstancedStructValue` _saveddata _structout))))

(fn `UserConstructionScript`
  (if (`self.bFlipRotation`)
    (set `self.FinalRotation` (`self.TargetRotation`))
    (`SceneComponent.K2_SetRelativeLocation` (`self.StaticMesh`) (0.0 -150.0 0.0) false false)
    (`SceneComponent.K2_SetRelativeRotation` :`self` (`self.Arrow`))
    (else
      (set `self.FinalRotation` (* (`self.TargetRotation`) -1.0))
      (`SceneComponent.K2_SetRelativeLocation` (`self.StaticMesh`) (-40.0 -150.0 0.0) false false)
      (`SceneComponent.K2_SetRelativeRotation` (`self.Arrow`) (struct :`Yaw` -180.0) false false))))