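; Environment event receiver component that wakes and spawns enemies when its trigger event plays.
; It revives living enemies in its awake list that are faking death, optionally setting the player as their AI combat target.
; It then tells each fan in its spawn list to spawn a Zero enemy from the configured data asset, passing along the auto-attack setting.
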(fn `OnPlayComponentSpecificEvent`
  (params (FromBoxEnter :type Boolean) (TriggerBox :type "Actor Object Reference"))
  (for _array_element (`self.EnemiesToAwake`)
    (`/Engine/EditorBlueprintResources/StandardMacros.IsValid` _array_element
      (:`Is Valid`
        (if (`HealthComponent.IsAlive` (`ZeroEnemy.HealthComponent` _array_element))
          (if (`|EnumEquality` (`ZeroEnemy.GetState` _array_element) "FakingDeath")
            (`ZeroEnemy.UnFakeDeath` _array_element)
            (if (`self.bAutoAttackPlayer`)
              (bind _aszero_enemy_aicontroller (cast `ZeroEnemyAIController` (`Pawn.GetController` _array_element)))
              (`ZeroEnemyAIController.CombatTarget` _aszero_enemy_aicontroller (`GameplayStatics.GetPlayerCharacter` 0))))))))
  (for _array_element_2 (`self.FansToSpawn`)
    (`/Game/Art/LevelPrototyping/Lights/BP_FanHighLight.SpawnEnemy` _array_element_2 (make `EnemySpawnerSpawnInfo` (`self.bAutoAttackPlayer`) "ZeroEnemy" (`self.ZeroEnemyDataAsset`)))))