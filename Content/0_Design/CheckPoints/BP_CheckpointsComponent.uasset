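; Actor component for a Character that records the last checkpoint transform, starting with the owner's transform at BeginPlay.
; SaveNewCheckpoint traces downward from the given transform, ignoring the owner, and lifts any ground hit by the cached capsule half-height.
; Without a hit it keeps the given location.
; The saved rotation is rebuilt upright from the forward vector, and scale is reset to one.
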(event `self.ReceiveBeginPlay`
  (set `self.CharacterCapsuleHalfHeight` (`CapsuleComponent.GetScaledCapsuleHalfHeight` (`Character.CapsuleComponent` (cast `Character` (`self.GetOwner`) :!pure true))))
  (`self.SaveNewCheckpoint` (`Actor.GetTransform` (`self.GetOwner`))))

(fn `SaveNewCheckpoint`
  (params (CheckpointTransform :type "Transform Structure"))
  (bind _returnvalue (`KismetMathLibrary.MakeRotFromXZ` (`KismetMathLibrary.GetForwardVector` CheckpointTransform_Rotation) (`KismetMathLibrary.Vector_Up`)))
  (bind (_outhit _returnvalue_2) (`KismetSystemLibrary.LineTraceSingle` (+ CheckpointTransform_Location (0.0 0.0 10.0)) (+ CheckpointTransform_Location (0.0 0.0 -1000.0)) "TraceTypeQuery5" false (`|MakeArray` (`self.GetOwner`))))
  (if _returnvalue_2
    (set `self.LastCheckpointTransform` (`KismetMathLibrary.MakeTransform` (+ (`.Location` (`GameplayStatics.BreakHitResult` _outhit)) (`KismetMathLibrary.MakeVector` 0.0 0.0 (`self.CharacterCapsuleHalfHeight`))) _returnvalue))
    (else
      (set `self.LastCheckpointTransform` (`KismetMathLibrary.MakeTransform` CheckpointTransform_Location _returnvalue)))))