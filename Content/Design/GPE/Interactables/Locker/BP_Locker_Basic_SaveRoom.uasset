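; An interactable save-room locker that can start open, half-open or locked, and holds an optional pickup.
; When locked, it spawns a lock actor in place of the preview and blocks interaction until the lock-down event half-opens the door.
; Interacting swings the door open at a random play rate, then unfreezes the pickup.
; The pickup spawns shortly after BeginPlay with random yaw; the overlap-based spawn is disconnected.
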(event `self.ReceiveBeginPlay`
  (`KismetSystemLibrary.DelayUntilNextTick`)
  (if (`self.bIsOpened`)
    (`self.SetInteractionFreezed` true)
    (elif (`self.bIsLocked`)
      (`self.SetupLock`)))
  (`self.SpawnPickup`))

(event `OnLockDown`
  (params (Lock :type "Lock Object Reference"))
  ;[1 1 1 0.33] Enable Interaction after shooting lock
  (`self.SetInteractionFreezed` false)
  (bind (_direction _doorrotation) (`Timeline|HalfOpenTimeline` :!via `PlayFromStart`)
    (:`Update`
      (`SceneComponent.K2_SetRelativeRotation` (`self.Door`) (`KismetMathLibrary.MakeRotator` 0.0 0.0 (`KismetMathLibrary.Lerp` 0.0 (`self.HalfOpenYawRotation`) _doorrotation)) false false)
      (`self.UpdateWidgetLocationToHandle`))))

(event `self.InteractableComponent.OnInteract`
  (bind _openanimationplayraterange (`self.OpenAnimationPlayRateRange`))
  (bind _door (`self.Door`))
  (bind (_relativerotation_roll _relativerotation_pitch _relativerotation_yaw) (`KismetMathLibrary.BreakRotator` (`SceneComponent.RelativeRotation` _door)))
  (`GameplayStatics.PlaySoundAtLocation` "/Game/Sounds/Audio/SD/MetaSounds/MS_Sources/GPE/Locker/MS_Locker_Open.MS_Locker_Open" (`SceneComponent.K2_GetComponentLocation` (`self.Door`)) (struct) 1.0 1.0 0.0 null null null null)
  (set `self.bIsOpened` true)
  (`self.SetInteractionFreezed` true)
  ;[1 1 1 0.33] Play Open Animation
  (`PrimitiveComponent.SetCollisionEnabled` _door "NoCollision")
  (bind _output_get (set `self.StartDoorYawRotation` _relativerotation_yaw))
  (`TimelineComponent.SetPlayRate` (`self.OpenDoorTimeline`) (`KismetMathLibrary.RandomFloatInRange` (`.Value` (break `FloatRangeBound` (break `FloatRange` _openanimationplayraterange))) (`.Value` (break `FloatRangeBound` (`.UpperBound` (break `FloatRange` _openanimationplayraterange))))))
  (bind (_direction _doorrotation) (`Timeline|OpenDoorTimeline` :`NewTime` 2.0 :!via `PlayFromStart`)
    (:`Update`
      (`SceneComponent.K2_SetRelativeRotation` (`self.Door`) (`KismetMathLibrary.MakeRotator` 0.0 0.0 (`KismetMathLibrary.Lerp` _output_get (`self.OpenYawRotation`) _doorrotation)) false false)
      (`self.UpdateWidgetLocationToHandle`))
    (:`Finished`
      (`PrimitiveComponent.SetCollisionEnabled` (`self.Door`) "QueryAndPhysics")
      ;[1 1 1 0.33] Enable interaction with Pickup
      (bind _pickup (`self.Pickup`)
        (:`then`
          (`self.SetInteractionFreezed` _pickup false))
        (:`else`)))))

(event `self.OutterCollision.OnComponentBeginOverlap`
  (params (OverlappedComponent :type "PrimitiveComponent Object Reference") (OtherActor :type "Actor Object Reference") (OtherComp :type "PrimitiveComponent Object Reference") (OtherBodyIndex :type Integer) (bFromSweep :type Boolean) (SweepResult :type "HitResult Structure (by ref)"))
  ;[0 0 0 0.33] DOP: Spawn only when entering OuterCollision
)

(fn `SetupLock`
  (bind (_returnvalue_location _returnvalue_rotation) (`KismetMathLibrary.BreakTransform` (`SceneComponent.K2_GetComponentToWorld` (`self.LockPreview`))))
  (bind _returnvalue (`|SpawnActorFromClass` "/Script/MetroXHunter.Lock" (`KismetMathLibrary.MakeTransform` _returnvalue_location _returnvalue_rotation) "Undefined" "MultiplyWithRoot" null null))
  (`self.K2_AttachToActor` _returnvalue self "None" "KeepWorld" "KeepWorld" "KeepWorld" true)
  (`StaticMeshComponent.SetStaticMesh` (`Lock.StaticMesh` _returnvalue) (`StaticMeshComponent.StaticMesh` (`self.LockPreview`)))
  (`ActorComponent.K2_DestroyComponent` (`self.LockPreview`))
  (add `Lock.OnLockDown` _returnvalue (`|CreateDelegate` :!event `OnLockDown`))
  (`self.SetInteractionFreezed` true))

(fn `SpawnPickup`
  (returns (Pickup :type "BasePickUp Object Reference"))
  (bind _itemrandomyawrotation (`self.ItemRandomYawRotation`))
  (bind _pickupspawnclass (`self.PickupSpawnClass`))
  (bind (_returnvalue_location _returnvalue_rotation) (`KismetMathLibrary.BreakTransform` (`SceneComponent.K2_GetComponentToWorld` (`self.ItemSpawnPoint`))))
  (if (`KismetSystemLibrary.IsValidClass` _pickupspawnclass)
    (bind _returnvalue (`|SpawnActorFromClass` _pickupspawnclass (`KismetMathLibrary.MakeTransform` _returnvalue_location (`KismetMathLibrary.ComposeRotators` _returnvalue_rotation (`KismetMathLibrary.MakeRotator` 0.0 0.0 (`KismetMathLibrary.RandomFloatInRange` (* _itemrandomyawrotation -1.0) _itemrandomyawrotation)))) "AdjustIfPossibleButAlwaysSpawn" "MultiplyWithRoot" null null))
    (`self.SetInteractionFreezed` _returnvalue (not (`self.bIsOpened`)))
    (bind _output_get (set `self.Pickup` _returnvalue))
    (return _output_get)))

(fn `UpdateWidgetLocationToHandle`
  (bind _handle (`self.Handle`))
  (`SceneComponent.K2_SetWorldLocation` (`self.Widget`) (+ (`SceneComponent.K2_GetComponentLocation` _handle) (* (`SceneComponent.GetUpVector` _handle) -5.0)) false false))

(fn `UserConstructionScript`
  (if (`self.bIsOpened`)
    (`SceneComponent.K2_SetRelativeRotation` (`self.Door`) (`KismetMathLibrary.MakeRotator` 0.0 0.0 (`self.OpenYawRotation`)) false false)
    (`ActorComponent.K2_DestroyComponent` (`self.LockPreview`))
    (else
      (if (not (`self.bIsLocked`))
        (`SceneComponent.K2_SetRelativeRotation` (`self.Door`) (`KismetMathLibrary.MakeRotator` 0.0 0.0 (`self.HalfOpenYawRotation`)) false false)
        (`ActorComponent.K2_DestroyComponent` (`self.LockPreview`)))
      (`self.UpdateWidgetLocationToHandle`))))