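; Environment event actor that moves an animated creature skeletal mesh along a spline when its trigger event receiver component fires.
; The mesh waits at the spline start, then Tick, switched on only during movement, advances it by elapsed time over spline duration with a rotation offset.
; At the end it either re-fires with a randomized, clamped duration or destroys itself.
; The Zero Enemy mesh also gets physics-simulated bones copied from that enemy's class defaults.
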(event `self.ReceiveBeginPlay`
  (`self.SetupSkeletalMesh`))

(event `self.ReceiveTick`
  (params (DeltaSeconds :type "Float (single-precision)"))
  (bind (_addon_rotation_roll _addon_rotation_pitch _addon_rotation_yaw) (`KismetMathLibrary.BreakRotator` (`self.Addon Rotation`)))
  (bind _returnvalue (`SplineComponent.GetTransformAtDistanceAlongSpline` (`self.Spline`) (* (`SplineComponent.GetSplineLength` (`self.Spline`)) (/ (`self.CurrentMovementTimer`) (`SplineComponent.Duration` (`self.Spline`)))) "Local" false))
  ;[0.5157 0.439 1 0.33] Advance the Skeletal Mesh on the Spline
  ; Later down the line we could put custom speeds, triggers at certain points and stuff, and much more.
  (bind _return (`/Game/Design/Libraries/BPL_GeneralUtilities.Increase Value Float` (`self.CurrentMovementTimer`) DeltaSeconds))
  (if (>= _return (`SplineComponent.Duration` (`self.Spline`)))
    (`self.EndSplineMovement`)
    (else
      (`SceneComponent.K2_SetRelativeLocationAndRotation` (`self.SkeletalMeshComponent`) (.location _returnvalue) (`KismetMathLibrary.MakeRotator` (+ (.roll (.rotation _returnvalue)) _addon_rotation_roll) (+ (.pitch (.rotation _returnvalue)) _addon_rotation_pitch) (+ (.yaw (.rotation _returnvalue)) _addon_rotation_yaw)) false false))))

(event `EndSplineMovement`
  (`SceneComponent.SetVisibility` (`self.SkeletalMeshComponent`) false false)
  (`self.SetActorTickEnabled` false)
  (if (`self.Loop`)
    (`/Game/Design/EnvironmentEvents/Components/BP_TriggerEventReceiver_Component.OnPlayComponentSpecificEvent` (`self.BP_CustomTriggerEventReceiver_Component`) false null)
    (set `self.CurrentMovementTimer` 0.0)
    (set `SplineComponent.Duration` (`KismetMathLibrary.FClamp` (+ (`self.SplineTotalDuration`) (`KismetMathLibrary.RandomFloatInRange` -1.0 1.0)) 8.0 14.0) (`self.Spline`))
    (else
      (`self.K2_DestroyActor`))))

(event `self.BP_CustomTriggerEventReceiver_Component.PlayComponentSpecificEvent_Dispatcher`
  ;[0.04835 0.1823 0.0471 0.33] Playing with the Tick itself instead of a Boolean.
  ; If for some reason a Boolean is needed instead, feel free to change the code
  (`SceneComponent.SetVisibility` (`self.SkeletalMeshComponent`) true false)
  (`self.SetActorTickEnabled` true)
  (`PrimitiveComponent.SetCollisionEnabled` (`self.SkeletalMeshComponent`) "QueryAndPhysics")
  (`SkeletalMeshComponent.Play` (`self.SkeletalMeshComponent`) true))

(fn `SetupSkeletalMesh`
  (bind (_curve_electrical_freeze _time_curve _knockbackdirection _legsbonenames _bshouldragdollfakedeath _boverridefakedeathanimation _fakedeathanimmontage _wartsdynamicmaterial _wartsparametername _wartsdefaultvalue _wartsnextmodifier _simulatedmeshbones _simulatedmeshbonesbelow) (defaults `/Game/Design/Enemies/AI/Zero/BP_ZeroEnemy` "/Game/Design/Enemies/AI/Zero/BP_ZeroEnemy.BP_ZeroEnemy_C"))
  ;[0.1236 0.349 0.06033 0.33] Place the Mesh at the start of the spline, hidden.
  (`SceneComponent.K2_SetRelativeLocation` (`self.SkeletalMeshComponent`) (`SplineComponent.GetLocationAtSplinePoint` (`self.Spline`) 0 "Local") false false)
  (`SceneComponent.SetVisibility` (`self.SkeletalMeshComponent`) (`self.isVisibleAtStart`) false)
  (`self.SetActorTickEnabled` false)
  (`SkeletalMeshComponent.Stop` (`self.SkeletalMeshComponent`))
  (if (== (`SkeletalMeshComponent.SkeletalMeshAsset` (`self.SkeletalMeshComponent`)) (`self.ZeroEnemySkeletalMesh`))
    (for _array_element _simulatedmeshbones
      (`SkeletalMeshComponent.SetBodySimulatePhysics` (`self.SkeletalMeshComponent`) _array_element true))
    (for _array_element_2 _simulatedmeshbonesbelow
      (`SkeletalMeshComponent.SetAllBodiesBelowSimulatePhysics` (`self.SkeletalMeshComponent`) _array_element_2 true true))))

(fn `UserConstructionScript`
  ;[0 0 0 0.33] Since nobody knows that Splines have their own "Duration" variable, let the LD make their own
  (set `SplineComponent.Duration` (`self.SplineTotalDuration`) (`self.Spline`)))