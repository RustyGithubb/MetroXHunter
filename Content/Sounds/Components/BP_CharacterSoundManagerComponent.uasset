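; Character sound manager component that plays footstep and flashlight switch sounds.
; On each footstep, a downward line trace from the owner finds the surface type, then a lookup picks a walk or run sound to play at the hit point.
; Rock is the default and also covers Beton, Gravel and Metal have their own sounds, and Water is a placeholder that only prints a message.
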(event `self.OnFootstep`
  (params (bIsRunning :type Boolean))
  (bind _returnvalue (`Actor.K2_GetActorLocation` (`self.GetOwner`)))
  ;[0.4281 0.3462 1 0.33 32] FOOTSTEP
  ;;[0.4281 0.3462 1 0.33] Raycast to the floor to determine surface type
  (bind (_outhit _returnvalue_2) (`KismetSystemLibrary.LineTraceSingle` _returnvalue (- _returnvalue (0.0 0.0 200.0)) "TraceTypeQuery1"))
  (if _returnvalue_2
    ;;[0.4281 0.3462 1 0.33] Play footstep sound depending on surface type
    (bind _footstepsound (`self.Get Foostep Sound` (`GameplayStatics.GetSurfaceType` _outhit) bIsRunning)) ; NOTE: This is in this function where you want to set your sounds references
    (`GameplayStatics.PlaySoundAtLocation` _footstepsound (`.Location` (`GameplayStatics.BreakHitResult` _outhit)) (struct) 1.0 1.0 0.0 null null null null)))

(event `self.OnFlashlightEnabled`
  (params (bIsActivated :type Boolean) (FlashlightLocation :type "Vector Structure"))
  ;[1 1 1 0.33 32] FLASHLIGHT
  (`GameplayStatics.PlaySoundAtLocation` "/Engine/VREditor/Sounds/UI/Flashlight_Switch.Flashlight_Switch" FlashlightLocation (struct) 1.0 1.0 0.0 null null null null))

(fn `Get Foostep Sound`
  (params (Selection :type "EPhysicalSurface Enum" :default "SurfaceType_Default") (bIsRunning :type Boolean))
  (returns (FootstepSound :type "SoundBase Object Reference"))
  (switch `EPhysicalSurface` Selection
    (:`SurfaceType_Default`
      _)
    (:`SurfaceType1`
      (`KismetSystemLibrary.PrintString` "CharacterSoundManager: Replace with water footstep sound")
      (return null))
    (:`SurfaceType2`
      _)
    (:`SurfaceType3`
      (return (select `bool` (`local.bIsRunning`) :`false` "/Game/Sounds/Audio/SFX/Character/Footsteps/Gravel/Walk/SC_Footsteps_Gravel_Walk.SC_Footsteps_Gravel_Walk" :`true` "/Game/Sounds/Audio/SFX/Character/Footsteps/Gravel/Run/SC_Footsteps_Gravel_Run.SC_Footsteps_Gravel_Run" :!type "SoundBase Object Reference")))
    (:`SurfaceType4`
      (return (select `bool` (`local.bIsRunning`) :`false` "/Game/Sounds/Audio/SFX/Character/Footsteps/Metal/Walk/SC_Footsteps_Metal_Walk.SC_Footsteps_Metal_Walk" :`true` "/Game/Sounds/Audio/SFX/Character/Footsteps/Metal/Run/SC_Footsteps_Metal_Run.SC_Footsteps_Metal_Run" :!type "SoundBase Object Reference"))))
  (return (select `bool` (`local.bIsRunning`) :`false` "/Game/Sounds/Audio/SFX/Character/Footsteps/Rock/Walk/SC_Footsteps_Rock_Walk.SC_Footsteps_Rock_Walk" :`true` "/Game/Sounds/Audio/SFX/Character/Footsteps/Rock/Run/SC_Footsteps_Rock_Run.SC_Footsteps_Rock_Run" :!type "SoundBase Object Reference")))