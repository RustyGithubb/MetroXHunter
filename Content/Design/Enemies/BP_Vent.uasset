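; BP_Vent is an enemy vent that acts as an entrance and spawn point, with a grid that blows off when used.
; Enemies entering or exiting trigger a one-time grid break that enables physics, applies a forward impulse and plays a reverberated metal sound.
; Player overlap requests enemy spawns once the VentManager's proximity timer depletes.
; Heard noise plays a scream if the manager counts enemies in the vent's zone.
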(event `self.ReceiveBeginPlay`
  (add `self.OnEnemyExit` (delegate `OnEnemyExit_Event`)))

(event `self.StartEnterVent`
  (params (Actor :type "Actor Object Reference"))
  (if (not (`self.bIsGridDestroyed`)) :!label _label
    (`self.Destroygrid`)))

(event `OnEnemyExit_Event` :!signature `self.OnEnemyExit`
  (params (SelfVent :type "Vent Object Reference") (Enemy :type "Actor Object Reference"))
  (goto _label))

(event `DestroyGrid`
  (bind _aerationgrid (`self.AerationGrid`))
  (`PrimitiveComponent.SetSimulatePhysics` _aerationgrid true)
  (`PrimitiveComponent.AddForce` _aerationgrid (* (`SceneComponent.GetForwardVector` _aerationgrid) 100000) "None" false)
  (set `self.bIsGridDestroyed` true)
  (`GameplayStatics.PlaySoundAtLocation` "/Game/Sounds/Audio/SFX/SFX_GPE/SFX_Vent/S_Vent_Sudden_Metal_SoundF.S_Vent_Sudden_Metal_SoundF" (`self.K2_GetActorLocation`) (struct) 1.0 1.0 0.0 "/Game/Sounds/Attenuations/SA_Reverb.SA_Reverb" null null null))

(event `self.Box.OnComponentBeginOverlap`
  (params (OverlappedComponent :type "PrimitiveComponent Object Reference") (OtherActor :type "Actor Object Reference") (OtherComp :type "PrimitiveComponent Object Reference") (OtherBodyIndex :type Integer) (bFromSweep :type Boolean) (SweepResult :type "HitResult Structure (by ref)"))
  (bind _ventmanager (`self.VentManager`))
  (`/Engine/EditorBlueprintResources/StandardMacros.IsValid` _ventmanager
    (:`Is Valid`
      (if (`VentManagerComponent.IsProximitySpawnTimerDepleted` _ventmanager)
        (`self.TrySpawnEnemies`)))))

(event `self.PawnSensing.OnHearNoise`
  (params (Instigator :type "Pawn Object Reference") (Location :type "Vector Structure (by ref)") (Volume :type "Float (single-precision)"))
  (if (> (`VentManagerComponent.GetEnemiesCounterInZone` (`self.VentManager`) (`self.Zone`)) 0)
    (`self.PlayScreamSound`)))

(fn `GetEntranceComponent`
  (returns (ReturnValue :type "SceneComponent Object Reference"))
  (return (`self.EntrancePoint`)))

(fn `GetSpawnPointComponent`
  (returns (ReturnValue :type "SceneComponent Object Reference"))
  (return (`self.SpawnPoint`)))

(fn `UserConstructionScript`)