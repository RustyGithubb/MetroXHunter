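; Playtest telemetry component that records player combat stats per checkpoint segment and saves them to CSV.
; ReceiveEvent tallies gameplay-tag events for deaths, shots, hits, dodges and reload outcomes, while AddDamageAmount totals damage by type.
; On a new checkpoint, level transition, quit, PIE end or debug key U, it writes stats, derived percentages and segment time to a timestamped file under Saved, then clears the stats.
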(event EventEndPlay
  (params (EndPlayReason :type EEndPlayReason%20Enum :default "Destroyed"))
  (switch Utilities|FlowControl|Switch|SwitchonEEndPlayReason EndPlayReason
    (:LevelTransition
      _)
    (:EndPlayInEditor
      _)
    (:Quit
      _))
  (CallFunction|ParseandSaveAllData))

(event EventBeginPlay
  (CallFunction|BindtoMultipleGameplayEvents "(GameplayTags=((TagName=\"Event.mainCharacter.Death\"),(TagName=\"Event.mainCharacter.Shoot\"),(TagName=\"Event.mainCharacter.ShotHit\"),(TagName=\"Event.SmallSpider.OnAttackJump\"),(TagName=\"Event.mainCharacter.SuccessfulDodge\"),(TagName=\"Event.ReloadSystem.StartReload\"),(TagName=\"Event.ReloadSystem.EndPerfectReload\"),(TagName=\"Event.ReloadSystem.EndFailedReload\"),(TagName=\"Event.ReloadSystem.EndActiveReload\")))" self)
  (Utilities|FlowControl|DelayUntilNextTick)
  (bind _output_get (Variables|Default|SetOwner (Components|GetOwner)))
  (Variables|Default|SetTimeAtLastCheckpoint (Actor|GetGameTimeSinceCreation _output_get)))

(event Input|KeyboardEvents|DebugKeyU
  (params (Key :type Key%20Structure :default "None") (ActionValue :type Input%20Action%20Value%20Structure))
  (:Pressed
    (CallFunction|ParseandSaveAllData)))

(fn ParseandSaveAllData
  (bind _returnvalue (Math|DateTime|Now))
  (bind _reloaddata (Variables|Default|GetReloadData))
  (bind _dodgedata (Variables|Default|GetDodgeData))
  (bind _bulletaccuracydata (Variables|Default|GetBulletAccuracyData))
  (bind _damagedata (Variables|Default|GetDamageData))
  (Variables|Default|SetDataToSave "")
  (Utilities|FlowControl|Sequence
    (:then_0
      ;[1 1 1 0.33] TimeSinceLastCheckpoint
      (bind _owner (Variables|Default|GetOwner)
        (:then
          (Variables|Default|SetGameTime (- (Actor|GetGameTimeSinceCreation _owner) (Variables|Default|GetTimeAtLastCheckpoint)))
          (Variables|Default|SetTimeAtLastCheckpoint (Actor|GetGameTimeSinceCreation (Variables|Default|GetOwner))))
        (:else)))
    (:then_1
      ;[1 1 1 0.33] Computer Session Name
      (CallFunction|AppendData (Utilities|String|Replace (Utilities|Platform|GetPlatformUserName) "leonard" "miya" "CaseSensitive"))
      ;[1 1 1 0.33] Date & Time
      (CallFunction|AppendData (Utilities|String|Replace (Utilities|String|ToString(Text) (Class|KismetTextLibrary|AsDateTimeDateTime (Math|DateTime|Now))) ","))
      ;[1 1 1 0.33] Checkpoint Number
      (CallFunction|AppendData (Utilities|String|ToString(Integer) (Variables|Default|GetCurrentCheckpointIndex)))
      ;[1 1 1 0.33] Game Since Checkpoint
      (CallFunction|AppendData (Utilities|String|ToString(Float) (Variables|Default|GetGameTime))))
    (:then_2
      ;[1 1 1 0.33] Bullet Accuracy
      (CallFunction|AppendData (Utilities|String|ToString(Integer) (.numberofbulletsshot _bulletaccuracydata)))
      (CallFunction|AppendData (Utilities|String|ToString(Integer) (.numberofbulletstouched _bulletaccuracydata)))
      (CallFunction|AppendData (Utilities|String|ToString(Float) (* (/ (Math|Conversions|ToFloat(Integer) (.numberofbulletstouched _bulletaccuracydata)) (Math|Conversions|ToFloat(Integer) (.numberofbulletsshot _bulletaccuracydata))) 1e+02))))
    (:then_3
      ;[1 1 1 0.33] Damage Data
      (CallFunction|AppendData (Utilities|String|ToString(Integer) (.damagefrommelee _damagedata)))
      (CallFunction|AppendData (Utilities|String|ToString(Integer) (.damagefromshock _damagedata)))
      (CallFunction|AppendData (Utilities|String|ToString(Integer) (.damagefromexplosion _damagedata))))
    (:then_4
      ;[1 1 1 0.33] Death Data
      (CallFunction|AppendData (Utilities|String|ToString(Integer) (.numberofdeaths (Variables|Default|GetDeathData)))))
    (:then_5
      ;[1 1 1 0.33] Dodge Data
      (CallFunction|AppendData (Utilities|String|ToString(Integer) (.numberofdodgeopportunities _dodgedata)))
      (CallFunction|AppendData (Utilities|String|ToString(Integer) (.numberofsuccessfuldodges _dodgedata)))
      (CallFunction|AppendData (Utilities|String|ToString(Float) (* (/ (Math|Conversions|ToFloat(Integer) (.numberofsuccessfuldodges _dodgedata)) (Math|Conversions|ToFloat(Integer) (.numberofdodgeopportunities _dodgedata))) 1e+02))))
    (:then_6
      ;[1 1 1 0.33] Reload Data
      (CallFunction|AppendData (Utilities|String|ToString(Integer) (.numberofreloads _reloaddata)))
      (CallFunction|AppendData (Utilities|String|ToString(Integer) (.numberoffailed _reloaddata)))
      (CallFunction|AppendData (Utilities|String|ToString(Integer) (.numberofactive _reloaddata)))
      (CallFunction|AppendData (Utilities|String|ToString(Integer) (.numberofperfect _reloaddata)))
      (CallFunction|AppendData (Utilities|String|ToString(Integer) (Utilities|Operators|Subtract (.numberofreloads _reloaddata) (.numberoffailed _reloaddata) (.numberofactive _reloaddata) (.numberofperfect _reloaddata))))
      (CallFunction|AppendData (Utilities|String|ToString(Float) (* (/ (Math|Conversions|ToFloat(Integer) (+ (.numberofactive _reloaddata) (.numberofperfect _reloaddata))) (Math|Conversions|ToFloat(Integer) (.numberofreloads _reloaddata))) 1e+02))))
    (:then_7
      (Class|MXHUtilityLibrary|SaveFileasString (Variables|Default|GetDataToSave) (Utilities|String|Append (Class|BlueprintPathsLibrary|ProjectSavedDir) "PlaytestTelemetry/" (Utilities|String|SelectString "PIE" "Build" (Class|MXHUtilityLibrary|IsWithinEditor)) "_Data_" (Utilities|String|ToString(Text) (Utilities|Text|FormatText "{day}-{month}_{hour}-{minute}-{seconds}" (Utilities|Text|ToText(Integer) (.day _returnvalue) false true 2) (Utilities|Text|ToText(Integer) (.month _returnvalue) false true 2) (Utilities|Text|ToText(Integer) (.hour _returnvalue) false true 2) (Utilities|Text|ToText(Integer) (.minute _returnvalue) false true 2) (Utilities|Text|ToText(Integer) (.second _returnvalue) false true 2))) "_Checkpoint" (Utilities|String|ToString(Integer) (Variables|Default|GetCurrentCheckpointIndex)) ".csv"))
      (CallFunction|ClearAllData))))

(fn AppendData
  (params (Data :type String))
  (Variables|Default|SetDataToSave (Utilities|String|Append (Variables|Default|GetDataToSave) Data ",")))

(fn ClearAllData
  (Variables|Default|SetBulletAccuracyData "")
  (Variables|Default|SetDamageData "")
  (Variables|Default|SetDeathData "")
  (Variables|Default|SetDodgeData "")
  (Variables|Default|SetReloadData "")
  (Variables|Default|SetDataToSave ""))

(fn AddDamageAmount
  (params (DamageValue :type Integer) (DamageType :type E_DamageType%20Enum :default "NewEnumerator2"))
  (switch Utilities|FlowControl|Switch|SwitchonE_DamageType DamageType
    (:NewEnumerator4
      (bind _structout (Utilities|Struct|SetmembersinS_TelemetryDamageData (Variables|Default|GetDamageData) (+ (.DamageFromMelee (Utilities|Struct|BreakS_TelemetryDamageData (Variables|Default|GetDamageData))) DamageValue)))
      (Variables|Default|SetDamageData _structout))
    (:NewEnumerator1
      (bind _structout_2 (Utilities|Struct|SetmembersinS_TelemetryDamageData (Variables|Default|GetDamageData) (+ (.DamageFromShock (Utilities|Struct|BreakS_TelemetryDamageData (Variables|Default|GetDamageData))) DamageValue)))
      (Variables|Default|SetDamageData _structout_2))
    (:NewEnumerator3
      (bind _structout_3 (Utilities|Struct|SetmembersinS_TelemetryDamageData (Variables|Default|GetDamageData) (+ (.DamageFromExplosion (Utilities|Struct|BreakS_TelemetryDamageData (Variables|Default|GetDamageData))) DamageValue)))
      (Variables|Default|SetDamageData _structout_3))))

(fn ReceiveNewCheckpoint
  (params (CheckpointIndex :type Integer))
  (CallFunction|ParseandSaveAllData)
  (Variables|Default|SetCurrentCheckpointIndex CheckpointIndex))

(fn ReceiveEvent
  (params (CalledTag :type Gameplay%20Tag%20Structure) (CallingObject :type Object%20Object%20Reference%20%28by%20ref%29))
  (|SwitchGameplayTag CalledTag
    (:Event.mainCharacter.Death
      (bind _structout (Utilities|Struct|SetmembersinS_TelemetryDeathData (Variables|Default|GetDeathData) (+ (Utilities|Struct|BreakS_TelemetryDeathData (Variables|Default|GetDeathData)) 1)))
      (Variables|Default|SetDeathData _structout))
    (:Event.mainCharacter.Shoot
      (bind _structout_2 (Utilities|Struct|SetmembersinS_TelemetryBulletAccuracy (Variables|Default|GetBulletAccuracyData) (+ (.NumberOfBulletsShot (Utilities|Struct|BreakS_TelemetryBulletAccuracy (Variables|Default|GetBulletAccuracyData))) 1)))
      (Variables|Default|SetBulletAccuracyData _structout_2))
    (:Event.mainCharacter.ShotHit
      (bind _structout_3 (Utilities|Struct|SetmembersinS_TelemetryBulletAccuracy (Variables|Default|GetBulletAccuracyData) (+ (.NumberOfBulletsTouched (Utilities|Struct|BreakS_TelemetryBulletAccuracy (Variables|Default|GetBulletAccuracyData))) 1)))
      (Variables|Default|SetBulletAccuracyData _structout_3))
    (:Event.mainCharacter.SuccessfulDodge
      (bind _structout_4 (Utilities|Struct|SetmembersinS_TelemetryDodgeData (Variables|Default|GetDodgeData) (+ (.NumberOfSuccessfulDodges (Utilities|Struct|BreakS_TelemetryDodgeData (Variables|Default|GetDodgeData))) 1)))
      (Variables|Default|SetDodgeData _structout_4))
    (:Event.SmallSpider.OnAttackJump
      (bind _structout_5 (Utilities|Struct|SetmembersinS_TelemetryDodgeData (Variables|Default|GetDodgeData) (+ (.NumberOfDodgeOpportunities (Utilities|Struct|BreakS_TelemetryDodgeData (Variables|Default|GetDodgeData))) 1)))
      (Variables|Default|SetDodgeData _structout_5))
    (:Event.ReloadSystem.StartReload
      (bind _structout_6 (Utilities|Struct|SetmembersinS_TelemetryReloadAcuracy (Variables|Default|GetReloadData) (+ (.NumberOfReloads (Utilities|Struct|BreakS_TelemetryReloadAcuracy (Variables|Default|GetReloadData))) 1)))
      (Variables|Default|SetReloadData _structout_6))
    (:Event.ReloadSystem.EndActiveReload
      (bind _structout_7 (Utilities|Struct|SetmembersinS_TelemetryReloadAcuracy (Variables|Default|GetReloadData) (+ (.NumberOfActive (Utilities|Struct|BreakS_TelemetryReloadAcuracy (Variables|Default|GetReloadData))) 1)))
      (Variables|Default|SetReloadData _structout_7))
    (:Event.ReloadSystem.EndFailedReload
      (bind _structout_8 (Utilities|Struct|SetmembersinS_TelemetryReloadAcuracy (Variables|Default|GetReloadData) (+ (.NumberOfFailed (Utilities|Struct|BreakS_TelemetryReloadAcuracy (Variables|Default|GetReloadData))) 1)))
      (Variables|Default|SetReloadData _structout_8))
    (:Event.ReloadSystem.EndPerfectReload
      (bind _structout_9 (Utilities|Struct|SetmembersinS_TelemetryReloadAcuracy (Variables|Default|GetReloadData) (+ (.NumberOfPerfect (Utilities|Struct|BreakS_TelemetryReloadAcuracy (Variables|Default|GetReloadData))) 1)))
      (Variables|Default|SetReloadData _structout_9))))