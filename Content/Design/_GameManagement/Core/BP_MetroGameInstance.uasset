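; Game instance for Metro that queues level streaming requests and loads them asynchronously, one at a time.
; A self-recursing event works through the unique-name queue behind a busy flag, since LoadStreamLevel cannot run concurrently, and signals each loaded level.
; Once the queue empties, a retriggerable delay debounces completion before the Metro game mode's light manager rescans the world for lights.
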(event `self.LoadLevelStreaming`
  (params (LevelName :type Name))
  (`KismetArrayLibrary.Array_AddUnique` (`self.LevelNamesToLoad`) LevelName)
  (`self.LoadNextStreamLevel`))

(event `LoadNextStreamLevel`
  (bind _levelnamestoload (`self.LevelNamesToLoad`))
  (bind _output (`|GetArrayItem` _levelnamestoload))
  (if (and (not (`self.bIsLevelStreamLoading`)) (`KismetArrayLibrary.Array_IsNotEmpty` (`self.LevelNamesToLoad`)))
    (set `self.bIsLevelStreamLoading` true)
    (`GameplayStatics.LoadStreamLevel` _output true)
    (`self.OnLevelStreamingLoad` _output)
    (set `self.bIsLevelStreamLoading` false)
    (`KismetArrayLibrary.Array_Remove` _levelnamestoload)
    (`self.LoadNextStreamLevel`)
    (if (`KismetArrayLibrary.Array_IsEmpty` _levelnamestoload)
      (`self.OnLevelStreamComplete`))))

(event `OnLevelStreamComplete`
  (`KismetSystemLibrary.RetriggerableDelay` 5.0)
  (bind _asbp_metro_game_mode (cast `/Game/Design/_GameManagement/Core/BP_MetroGameMode` (`GameplayStatics.GetGameMode`))
    (:`then`
      (`LightManagerComponent.FindAllLightsInWorld` (`/Game/Design/_GameManagement/Core/BP_MetroGameMode.LightManager` _asbp_metro_game_mode)) ; TODO: Make lights register themselves to the manager\nMake a specific component for this?
    )
    (:`CastFailed`
      (`KismetSystemLibrary.PrintString` "GameInstance: Gamemode is not of the correct class!" true true (struct :`R` 1.0 :`A` 1.0) 10.0))))