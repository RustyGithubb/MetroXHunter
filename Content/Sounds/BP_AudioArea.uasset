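; BP_AudioArea is a trigger volume that switches the player's ambient loop when BP_MainChara enters its box.
; After validating both audio tracks on the character, it uses the EAmbiances value to set and activate a sound cue.
; Manif and Staff Area play on AudioTrack1, Tunnel on AudioTrack2, with debug prints throughout.
; Nothing stops the other track: CrossFade, FadeIn and FadeOut are empty, and the fade logic is unwired.
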(event `CrossFade`)

(event `FadeOut`)

(event `FadeIn`)

(event `self.Box.OnComponentBeginOverlap`
  (params (OverlappedComponent :type "PrimitiveComponent Object Reference") (OtherActor :type "Actor Object Reference") (OtherComp :type "PrimitiveComponent Object Reference") (OtherBodyIndex :type Integer) (bFromSweep :type Boolean) (SweepResult :type "HitResult Structure (by ref)"))
  (bind _audiotrack2 (`/Game/Design/_GameManagement/BP_MainChara.AudioTrack2` (`self.RefMainChara`)))
  (bind _audiotrack1 (`/Game/Design/_GameManagement/BP_MainChara.AudioTrack1` (`self.RefMainChara`)))
  (bind _audiotrack1_2 (`/Game/Design/_GameManagement/BP_MainChara.AudioTrack1` (`self.RefMainChara`)))
  ;[0.4675 0.2974 1 0.33 30] Setup Ref
  (bind _asbp_main_chara (cast `/Game/Design/_GameManagement/BP_MainChara` OtherActor))
  (bind _output_get (set `self.RefMainChara` _asbp_main_chara))
  (`/Engine/EditorBlueprintResources/StandardMacros.IsValid` (`/Game/Design/_GameManagement/BP_MainChara.AudioTrack1` _output_get)
    (:`Is Valid`
      (`/Engine/EditorBlueprintResources/StandardMacros.IsValid` (`/Game/Design/_GameManagement/BP_MainChara.AudioTrack2` _output_get)
        (:`Is Valid`
          (switch `/Game/Sounds/E_Ambiances` (`self.EAmbiances`)
            (:`NewEnumerator0`
              (`KismetSystemLibrary.PrintString` "Manif" true true (struct :`R` 1.0 :`G` 0.54418 :`A` 1.0))
              (`AudioComponent.SetSound` _audiotrack1 "/Game/Sounds/Audio/Ambient/Areas/SC_Ambient_Manifestation_Loop.SC_Ambient_Manifestation_Loop")
              (`ActorComponent.Activate` _audiotrack1 false))
            (:`NewEnumerator1`
              (`KismetSystemLibrary.PrintString` "Tunnel" true true (struct :`R` 1.0 :`G` 0.54418 :`A` 1.0))
              (`AudioComponent.SetSound` _audiotrack2 "/Game/Sounds/Audio/Ambient/Areas/SC_Ambient_Tunnels_Loop.SC_Ambient_Tunnels_Loop")
              (`ActorComponent.Activate` _audiotrack2 false))
            (:`NewEnumerator2`
              (`KismetSystemLibrary.PrintString` "Staff Area" true true (struct :`R` 1.0 :`G` 0.54418 :`A` 1.0))
              (`AudioComponent.SetSound` _audiotrack1_2 "/Game/Sounds/Audio/Ambient/Areas/SC_Ambient_StaffArea_Loop.SC_Ambient_StaffArea_Loop")
              (`ActorComponent.Activate` _audiotrack1_2 false))))
        (:`Is Not Valid`
          (`KismetSystemLibrary.PrintString` "BP_AudioArea -> BP_Chara -> AudioTrack2 Not Valid" true true (struct :`R` 1.0 :`G` 0.54418 :`A` 1.0)))))
    (:`Is Not Valid`
      (`KismetSystemLibrary.PrintString` "BP_AudioArea -> BP_Chara -> AudioTrack1 Not Valid" true true (struct :`R` 1.0 :`G` 0.54418 :`A` 1.0)))))

(fn `UserConstructionScript`)