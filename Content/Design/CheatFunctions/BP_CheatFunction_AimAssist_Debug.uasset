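; Cheat function that toggles the debug mode of the aim assist component on the player's controlled pawn.
; On init it waits one tick, then caches the AimAssistComponent from the pawn controlled by the cheat manager's player controller.
; When triggered, and only if that component is enabled, it copies the toggle state to the component's debug flag and calls InitializeHUD on it.
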(event `self.OnInit`
  (`KismetSystemLibrary.DelayUntilNextTick`)
  (`self.GetReferences`))

(event `self.OnCheat`
  (bind _aimassistcomponent (`self.AimAssistComponent`))
  (if (`/AdvancedAimAssist/Blueprints/Components/AAA_BP_AimAssistComponent.bIsComponentEnable` _aimassistcomponent)
    (set `/AdvancedAimAssist/Blueprints/Components/AAA_BP_AimAssistComponent.bIsDebugActivated` (`self.bIsToggled`) _aimassistcomponent)
    (`/AdvancedAimAssist/Blueprints/Components/AAA_BP_AimAssistComponent.Initialize HUD` _aimassistcomponent)))

(fn `GetReferences`
  (bind _returnvalue (`Controller.K2_GetPawn` (`CheatManager.GetPlayerController` (`self.CheatManager`))))
  (`/Engine/EditorBlueprintResources/StandardMacros.IsValid` _returnvalue
    (:`Is Valid`
      (set `self.AimAssistComponent` (`Actor.GetComponentByClass` _returnvalue "/AdvancedAimAssist/Blueprints/Components/AAA_BP_AimAssistComponent.AAA_BP_AimAssistComponent_C")))))