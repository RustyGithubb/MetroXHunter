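; BP_Water_Interactions is an actor that acts as a moving force source for the water fluid simulation.
; On BeginPlay, after a short delay, it finds BP_FluidSim_01 and registers ForceMesh as a dynamic force with configurable radius, strength and material.
; Tick oscillates the mesh along its relative X axis with a time-based sine.
; The construction script scales the mesh to the radius and sets its in-game visibility.
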(event `self.ReceiveTick`
  (params (DeltaSeconds :type "Float (single-precision)"))
  (`SceneComponent.K2_SetRelativeLocation` (`self.ForceMesh`) (`KismetMathLibrary.MakeVector` (* (`KismetMathLibrary.Sin` (* (`KismetSystemLibrary.GetGameTimeInSeconds`) (`self.Oscillation Speed`))) (`self.Osc Mag`))) false false))

(event `self.ReceiveBeginPlay`
  (bind _sim (`self.Sim`))
  (`KismetSystemLibrary.Delay` 0.1)
  (bind _returnvalue (`GameplayStatics.GetActorOfClass` "/Water/FluidSimulation/Blueprints/BP_FluidSim_01.BP_FluidSim_01_C"))
  (set `self.Sim` _returnvalue)
  (`/Engine/EditorBlueprintResources/StandardMacros.IsValid` _sim
    (:`Is Valid`
      (`/Water/FluidSimulation/Blueprints/BP_FluidSim_01.Register Dynamic Force` _sim (make `/Water/FluidSimulation/Blueprints/Structs/FluidForceDynamic` "NewEnumerator0" (`self.Radius`) (`self.Strength`) (`self.ForceMesh`) (`self.Material`) (make `/Water/FluidSimulation/Blueprints/Structs/FluidForceSocketInfo` (`|MakeMap` "None" :!type "Name" :!valuetype "Name"))) (`self.ForceMesh`) 0.0))))

(fn `UserConstructionScript`
  (`SceneComponent.SetWorldScale3D` (`self.ForceMesh`) (`KismetMathLibrary.Conv_DoubleToVector` (* (`self.Radius`) 1.0)))
  (`SceneComponent.SetHiddenInGame` (`self.ForceMesh`) (not (`self.Show Mesh`)) false))