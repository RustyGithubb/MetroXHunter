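; Damage volume that periodically hurts every overlapping actor that has a HealthComponent.
; Overlap events maintain the list of targets and toggle a Tick-driven cooldown, which applies typed damage to all of them whenever it elapses.
; Shock damage also electrocutes owners with an ElectrocutableComponent for the cooldown's duration.
; A known bug remains: overlap changes on Parasite death can modify the list during the damage loop.
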(event `self.ReceiveTick`
  (params (DeltaSeconds :type "Float (single-precision)"))
  (bind _currentcooldown (`self.CurrentCooldown`))
  (if (`self.IsBoxTriggered`)
    (`/Game/Design/Libraries/BPL_GeneralUtilities.Increase Value Float` _currentcooldown DeltaSeconds)
    (if (>= _currentcooldown (`self.DamageCooldown`))
      (`self.ApplyContinuousDamage`))))

(event `self.CollisionComponent.OnComponentBeginOverlap`
  (params (OverlappedComponent :type "PrimitiveComponent Object Reference") (OtherActor :type "Actor Object Reference") (OtherComp :type "PrimitiveComponent Object Reference") (OtherBodyIndex :type Integer) (bFromSweep :type Boolean) (SweepResult :type "HitResult Structure (by ref)"))
  (bind _returnvalue (`self.GetComponentByClass` OtherActor "/Script/MetroXHunter.HealthComponent"))
  (`/Engine/EditorBlueprintResources/StandardMacros.IsValid` _returnvalue
    (:`Is Valid`
      (`KismetArrayLibrary.Array_Add` (`self.HealthComponent`) _returnvalue)
      (set `self.IsBoxTriggered` true))))

(event `self.CollisionComponent.OnComponentEndOverlap`
  (params (OverlappedComponent :type "PrimitiveComponent Object Reference") (OtherActor :type "Actor Object Reference") (OtherComp :type "PrimitiveComponent Object Reference") (OtherBodyIndex :type Integer))
  (bind _returnvalue (`self.GetComponentByClass` OtherActor "/Script/MetroXHunter.HealthComponent"))
  (`/Engine/EditorBlueprintResources/StandardMacros.IsValid` _returnvalue
    (:`Is Valid`
      (`KismetArrayLibrary.Array_RemoveItem` (`self.HealthComponent`) _returnvalue)
      (if (`KismetArrayLibrary.Array_IsEmpty` (`self.HealthComponent`))
        (set `self.IsBoxTriggered` false)
        (set `self.CurrentCooldown` 0.9)))))

(fn `ApplyContinuousDamage`
  (bind _damagetype (`self.DamageType`))
  (set `self.CurrentCooldown` 0.0)
  (for _array_element (`self.HealthComponent`)
    (`HealthComponent.TakeDamage` _array_element (make `DamageContext` null (`self.DamageAmount`) _damagetype self self))
    (switch `EDamageType` _damagetype
      (:`Shock`
        (bind _returnvalue (`ActorComponent.GetOwner` _array_element))
        ;[1 1 1 0.33] Extra logic for electrocuting the player with Shock damage
        ; TODO: Move this in the player's OnDamage event or find a generic way to trigger electricity
        (`/Engine/EditorBlueprintResources/StandardMacros.IsValid` _returnvalue
          (:`Is Valid`
            (bind _returnvalue_2 (`self.GetComponentByClass` _returnvalue "/Script/MetroXHunter.ElectrocutableComponent"))
            (`/Engine/EditorBlueprintResources/StandardMacros.IsValid` _returnvalue_2
              (:`Is Valid`
                (`ElectrocutableComponent.Electrocute` _returnvalue_2 (`self.DamageCooldown`))))))))))

(fn `UserConstructionScript`)