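; Cheat function that toggles camera collision debugging on the player's spring arm addon.
; On init it waits one tick, then caches the BPAC_SpringArmAddon component from the controlled pawn of the cheat manager's player controller.
; When the cheat fires, it copies its toggle state into the component's DebugLog flag, using the cached reference without a validity check.
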(event `self.OnInit`
  (`KismetSystemLibrary.DelayUntilNextTick`)
  (`self.GetReferences`))

(event `self.OnCheat`
  (set `/TPS_FeedlingAddon/TPS/BPAC_SpringArmAddon.DebugLog` (`self.bIsToggled`) (`self.SpringArmAddon`)))

(fn `GetReferences`
  (bind _returnvalue (`Controller.K2_GetPawn` (`CheatManager.GetPlayerController` (`self.CheatManager`))))
  (`/Engine/EditorBlueprintResources/StandardMacros.IsValid` _returnvalue
    (:`Is Valid`
      (set `self.SpringArmAddon` (`Actor.GetComponentByClass` _returnvalue "/TPS_FeedlingAddon/TPS/BPAC_SpringArmAddon.BPAC_SpringArmAddon_C")))))