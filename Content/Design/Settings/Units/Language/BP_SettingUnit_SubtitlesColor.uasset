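; BP_SettingUnit_SubtitlesColor is a language settings unit that sets the subtitle text color from a preset list.
; When the setting is applied in game, it writes the preset at the selected index to the dialogue subtitles inside WBP_Viewport.
; If no valid viewport reference is cached, it only looks up and stores the first WBP_Viewport, without applying the color on that call.
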(event `self.OnApplySetting`
  (params (bInGame :type Boolean))
  (bind _viewport (`self.Viewport`))
  (if bInGame
    (`/Engine/EditorBlueprintResources/StandardMacros.IsValid` _viewport
      (:`Is Valid`
        (set `TextBlock.ColorAndOpacity` (`|GetArrayItem` (`self.ColorsPreset`) (`self.IndexValue`)) (`/Game/Design/Widgets/Subtitles/WBP_Dialogue.Subtitles` (`/Game/Design/Widgets/WBP_Viewport.WBP_Dialogue` _viewport))))
      (:`Is Not Valid`
        (bind _foundwidgets (`WidgetBlueprintLibrary.GetAllWidgetsOfClass` "/Game/Design/Widgets/WBP_Viewport.WBP_Viewport_C" false))
        (set `self.Viewport` (`|GetArrayItem` _foundwidgets))))))