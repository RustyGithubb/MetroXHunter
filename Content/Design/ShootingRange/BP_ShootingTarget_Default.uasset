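; Shooting range target that drops when its Health component reports death, then resets itself after a delay.
; Death disables collision and plays a timeline tipping the support; the reset restores collision and health and reverses the timeline.
; Optionally, Tick shuttles the base between its start and a target position at a frame-dependent speed, pausing at each end.
; The construction script previews that path with a debug line.
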(event `self.ReceiveBeginPlay`
  (set `self.OriginPosition` (`SceneComponent.K2_GetComponentLocation` (`self.Base`))))

(event `self.Health.OnDeath`
  (params (DamageContext :type "DamageContext Structure (by ref)"))
  ;[1 0 0.02318 0.5] ONDEATH
  (`PrimitiveComponent.SetCollisionEnabled` (`self.Target`) "NoCollision")
  (`|ExecutionSequence`
    (:`then_0`
      ;;[1 1 1] Rotate the Target
      (bind (_direction _rotationx) (`Timeline|Timeline` :!via `PlayFromStart` :!label _label)
        (:`Update`
          (`SceneComponent.K2_SetRelativeRotation` (`self.Support`) (`KismetMathLibrary.MakeRotator` (* _rotationx -90.0)) false false))))
    (:`then_1`
      (`KismetSystemLibrary.Delay` (`self.DelayBetweenReset`))
      (`self.ResetTarget`)
      (`HealthComponent.Reset` (`self.Health`))
      (goto _label :!via `ReverseFromEnd`))))

(event `self.ReceiveTick`
  (params (DeltaSeconds :type "Float (single-precision)"))
  ;[0.5553 1 0 0.25] MOVING TARGET
  (if (`self.IsMovingTarget`)
    ;;[1 1 1] Move to target
    (`SceneComponent.K2_AddWorldOffset` (`self.Base`) (* (`KismetMathLibrary.GetDirectionUnitVector` (`SceneComponent.K2_GetComponentLocation` (`self.Base`)) (`self.NextPosition`)) (`self.Speed`)) false false)
    ;;[1 1 1] Set Next Target Position
    (if (<= (`KismetMathLibrary.Vector_Distance` (`self.NextPosition`) (`SceneComponent.K2_GetComponentLocation` (`self.Base`))) (`self.Speed`))
      (`self.SetNextPosition`)
      ;;[1 1 1] Delay when reaching target
      (set `self.IsMovingTarget` false)
      (`KismetSystemLibrary.Delay` (`self.TimeBeforeNextPos`))
      (set `self.IsMovingTarget` true))))

(fn `ResetTarget`
  (`PrimitiveComponent.SetCollisionEnabled` (`self.Target`) "QueryAndPhysics")
  (`HealthComponent.Reset` (`self.Health`)))

(fn `SetNextPosition`
  (locals (LastPosition :type "Vector Structure" :default (0.0 0.0 0.0)))
  (set `local.LastPosition` (`self.NextPosition`))
  (set `self.NextPosition` (`self.OriginPosition`))
  (set `self.OriginPosition` (`local.LastPosition`)))

(fn `UserConstructionScript`
  (if (`self.IsMovingTarget`)
    ;[1 1 1] Draw Line
    (`KismetSystemLibrary.FlushPersistentDebugLines`)
    (bind _output_get (set `self.NextPosition` (`KismetMathLibrary.TransformLocation` (`self.GetTransform`) (`self.TargetPosition`))))
    (`KismetSystemLibrary.DrawDebugLine` (`SceneComponent.K2_GetComponentLocation` (`self.Base`)) _output_get (struct :`A` 1.0) 10.0 10.0)
    (else
      ;[1 1 1] Delet Lines
      (`KismetSystemLibrary.FlushPersistentDebugLines`))))