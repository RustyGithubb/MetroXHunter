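; Blood puddle decal Blueprint that animates a dissolve effect on a decal material.
; The construction script picks a random material from an array, applies scale with X and Z swapped, and creates a dynamic instance.
; On BeginPlay, one-shot mode plays the Accumulate timeline in reverse to drive the Dissolve parameter.
; Otherwise, the Burst timeline drives it forward, with a timer scheduling PlayVFX again when FireRate is positive.
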(event `self.ReceiveBeginPlay`
  (bind _firerate (`self.FireRate`))
  (if (`self.IsOneShot`)
    (`TimelineComponent.SetPlayRate` (`self.Accumulate_Curve`) (`self.PlayRate`))
    (bind (_direction _curve) (`Timeline|Accumulate_Curve` :!via `ReverseFromEnd`)
      (:`Update`
        (`MaterialInstanceDynamic.SetScalarParameterValue` (`self.DynamicDecal`) "Dissolve" _curve)))
    (else
      (`self.PlayVFX`)
      (if (> _firerate 0.0)
        (`KismetSystemLibrary.K2_SetTimerDelegate` (delegate `PlayVFX`) _firerate)))))

(event `PlayVFX`
  (`TimelineComponent.SetPlayRate` (`self.Burst_Curve`) (`self.PlayRate`))
  (bind (_direction _curve) (`Timeline|Burst_Curve` :!via `PlayFromStart`)
    (:`Update`
      (`MaterialInstanceDynamic.SetScalarParameterValue` (`self.DynamicDecal`) "Dissolve" _curve))))

(fn `UserConstructionScript`
  (bind (_scale_x _scale_y _scale_z) (`KismetMathLibrary.BreakVector` (`self.Scale`)))
  (`DecalComponent.SetDecalMaterial` (`self.Decal`) (`|GetArrayItem` (`self.DecalMaterial`) (`KismetMathLibrary.RandomIntegerInRange` 0 3)))
  (`SceneComponent.SetRelativeScale3D` (`self.Decal`) (`KismetMathLibrary.MakeVector` _scale_z _scale_y _scale_x))
  (bind _returnvalue (`DecalComponent.CreateDynamicMaterialInstance` (`self.Decal`)))
  (set `self.DynamicDecal` _returnvalue))