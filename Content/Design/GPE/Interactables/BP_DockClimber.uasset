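; Spline-based interactable that lets the player climb onto a dock by teleporting behind a screen fade.
; Each Tick it enables interaction only while the player is grounded below the actor, sliding the widget and collisions to the closest spline point.
; Interacting stops aiming, suspends input during the fade, then places the player at that point, offset sideways and raised.
; The construction script previews landing spots with arrows along the spline.
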(event `self.ReceiveTick`
  (params (DeltaSeconds :type "Float (single-precision)"))
  (bind (_returnvalue_x _returnvalue_y _returnvalue_z) (`KismetMathLibrary.BreakVector` (`self.K2_GetActorLocation`)))
  (bind _returnvalue (`GameplayStatics.GetPlayerCharacter` 0))
  (bind _currentsplinetransform_location (`KismetMathLibrary.BreakTransform` (`self.CurrentSplineTransform`)))
  (bind (_returnvalue_x_2 _returnvalue_y_2 _returnvalue_z_2) (`KismetMathLibrary.BreakVector` (`self.K2_GetActorLocation` _returnvalue)))
  (`/Engine/EditorBlueprintResources/StandardMacros.IsValid` _returnvalue
    (:`Is Valid`
      (if (and (not (`NavMovementComponent.IsFalling` (`Character.CharacterMovement` _returnvalue))) (< _returnvalue_z_2 _returnvalue_z))
        (`self.SetInteractionFreezed` false)
        (set `self.CurrentSplineTransform` (`SplineComponent.FindTransformClosestToWorldLocation` (`self.Spline`) (`self.K2_GetActorLocation` (`GameplayStatics.GetPlayerCharacter` 0)) "Local" false))
        (`SceneComponent.K2_SetRelativeLocation` (`self.Widget`) _currentsplinetransform_location false false)
        (`SceneComponent.K2_SetRelativeLocation` (`self.OutterCollision`) _currentsplinetransform_location false false)
        (`SceneComponent.K2_SetRelativeLocation` (`self.InnerCollision`) _currentsplinetransform_location false false)
        (else
          (`self.SetInteractionFreezed` true))))))

(event `self.InteractableComponent.OnInteract`
  (bind _returnvalue (`GameplayStatics.GetPlayerController` 0))
  (bind _blackfader (`/Game/Design/Widgets/WBP_Viewport.BlackFader` (`/Game/Design/_GameManagement/Core/BP_MetroHUD.Viewport` (cast `/Game/Design/_GameManagement/Core/BP_MetroHUD` (`PlayerController.GetHUD` _returnvalue) :!pure true))))
  (`BaseMetroPlayerCharacter.StopAiming` (cast `MetroPlayerCharacter` (`GameplayStatics.GetPlayerCharacter` 0) :!pure true))
  (message `PlayerInputHandler.SetInputMappingContext` _returnvalue "/Game/Design/_GameManagement/Input/Player/IMC_None.IMC_None")
  (`/Game/Design/Widgets/WBP_BlackFader.Fade` _blackfader 1.0 true)
  (`KismetSystemLibrary.Delay` 1.0)
  (`/Game/Design/Widgets/WBP_BlackFader.Fade` _blackfader 1.0 false)
  (message `PlayerInputHandler.ResetInputMappingContext` _returnvalue)
  (`self.K2_SetActorLocation` (`GameplayStatics.GetPlayerCharacter` 0) (`self.ComputeCharacterSpawnLocation`) false true))

(fn `ComputeCharacterSpawnLocation`
  (returns (SpawnLocation :type "Vector Structure"))
  (bind _returnvalue (`self.GetTransform`))
  (bind (_currentsplinetransform_location _currentsplinetransform_rotation) (`KismetMathLibrary.BreakTransform` (`self.CurrentSplineTransform`)))
  (bind (_spawnlocation_x _spawnlocation_y _spawnlocation_z) (`KismetMathLibrary.BreakVector` (`self.GetSpawnLocationFromSplineLocation` (`KismetMathLibrary.MakeTransform` (`KismetMathLibrary.TransformLocation` _returnvalue _currentsplinetransform_location) (`KismetMathLibrary.TransformRotation` _returnvalue _currentsplinetransform_rotation)))))
  (return (`KismetMathLibrary.MakeVector` _spawnlocation_x _spawnlocation_y (+ _spawnlocation_z 90.0))))

(fn `GetSpawnLocationFromSplineLocation`
  (params (PointTransform :type "Transform Structure"))
  (returns (SpawnLocation :type "Vector Structure"))
  (return (+ PointTransform_Location (* (`KismetMathLibrary.GetRightVector` PointTransform_Rotation) (`self.ClimbDockSpacing`)))))

(fn `UserConstructionScript`
  (bind _previewspacing (`self.PreviewSpacing`))
  (for _index (range (+ (`KismetMathLibrary.FTrunc` (/ (`SplineComponent.GetSplineLength` (`self.Spline`)) _previewspacing)) 1))
    (`AddComponent|NODE_AddArrowComponent-0` :`RelativeTransform` (`KismetMathLibrary.MakeTransform` (- (`self.GetSpawnLocationFromSplineLocation` (`SplineComponent.GetTransformAtDistanceAlongSpline` (`self.Spline`) (* _index _previewspacing) "World" false)) (`self.K2_GetActorLocation`)) (struct :`Pitch` 90.0)))))