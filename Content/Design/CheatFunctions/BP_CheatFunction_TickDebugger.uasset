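; Cheat function that shows per-tick debug text above the player's pawn for a selected TickDebugger object.
; On init, after a one-tick delay, it lists TickDebugger implementers among the player controller, pawn, game mode and their components, plus a "None" option.
; A console variable stores the chosen object's name when the cheat fires and restores the selection on init.
; Each tick draws the selected object's TickDebugMessage as a debug string.
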(event `self.OnInit`
  (bind _returnvalue (`CheatManager.GetPlayerController` (`self.CheatManager`)))
  (`KismetSystemLibrary.DelayUntilNextTick`)
  (`self.AddDebuggingObjectsOf` _returnvalue)
  (`self.AddDebuggingObjectsOf` (`Controller.K2_GetPawn` _returnvalue))
  (`self.AddDebuggingObjectsOf` (`GameplayStatics.GetGameMode`))
  (`KismetArrayLibrary.Array_Add` (`self.ValueNames`))
  (for (_array_element _array_index) (`self.DebuggingObjects`)
    (bind _returnvalue_2 (`KismetSystemLibrary.GetObjectName` _array_element))
    (`KismetArrayLibrary.Array_Add` (`self.ValueNames`) _returnvalue_2)
    ;[1 1 1 0.33] Find default debuggin object
    (if (== _returnvalue_2 (`ConvarLibrary.GetTickDebuggerDefaultNameConvarValue`))
      (set `self.Index` (+ _array_index 1)))))

(event `self.OnCheat`
  (bind _debuggingobject (`self.GetCurrentDebuggingObject`))
  (`/Engine/EditorBlueprintResources/StandardMacros.IsValid` _debuggingobject
    (:`Is Valid`
      (`ConvarLibrary.SetTickDebuggerDefaultNameConvarValue` (`KismetSystemLibrary.GetObjectName` _debuggingobject)))
    (:`Is Not Valid`
      (`ConvarLibrary.SetTickDebuggerDefaultNameConvarValue` ""))))

(event `self.OnTick`
  (params (DeltaTime :type "Float (single-precision)"))
  (bind _debuggingobject (`self.GetCurrentDebuggingObject`))
  (`/Engine/EditorBlueprintResources/StandardMacros.IsValid` _debuggingobject
    (:`Is Valid`
      (bind _outdebugtext (message `TickDebugger.TickDebug` _debuggingobject DeltaTime))
      (`KismetSystemLibrary.DrawDebugString` (0.0 0.0 50.0) _outdebugtext (`Controller.K2_GetPawn` (`CheatManager.GetPlayerController` (`self.CheatManager`)))))))

(fn `AddDebuggingObjectsOf`
  (params (Actor :type "Actor Object Reference"))
  (`/Engine/EditorBlueprintResources/StandardMacros.IsValid` Actor
    (:`Is Valid`
      (`KismetArrayLibrary.Array_Append` (`self.DebuggingObjects`) (`Actor.GetComponentsByInterface` Actor "/Script/MetroXHunter.TickDebugger"))
      (if (`KismetSystemLibrary.DoesImplementInterface` Actor "/Script/MetroXHunter.TickDebugger")
        (`KismetArrayLibrary.Array_Add` (`self.DebuggingObjects`) Actor)))))

(fn `GetCurrentDebuggingObject`
  (returns (DebuggingObject :type "Object Object Reference"))
  (bind _returnvalue (- (`self.Index`) 1))
  (if (!= _returnvalue -1)
    (return (`|GetArrayItem` (`self.DebuggingObjects`) _returnvalue))
    (else
      (return null))))