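; HUD that creates the main WBP_Viewport widget and acts as the gateway to the game's on-screen UI.
; On BeginPlay it adds the viewport, then initializes child widgets a tick later as a stopgap for proper init ordering.
; Its functions forward prompts, indications, ammo, reload QTE and locker skill check updates to child widgets.
; A successful locker press fires a tagged gameplay event; the cheat menu is created on first show.
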(event `self.ReceiveBeginPlay`
  (bind _returnvalue (`|CreateWidget` "/Game/Design/Widgets/WBP_Viewport.WBP_Viewport_C"))
  (bind _output_get (set `self.Viewport` _returnvalue))
  (`UserWidget.AddToViewport` _output_get 0)
  ;[0.2812 0.04834 0.1037] Please, change this at some point to only initialize the HUD when the rest is initialized; not just a random Delay...
  (`KismetSystemLibrary.DelayUntilNextTick`)
  (`/Game/Design/Widgets/WBP_Viewport.InitializeChildrenWidgets` (`self.Viewport`)))

(fn `GiveInputToLockerSkillCheck`
  (params (MovementInputs :type "Vector2D Structure"))
  (returns (Return :type Boolean))
  (`/Game/Design/Widgets/Interactions/WBP_LockerSkillCheck.UpdateJoystickVisualizer` (`/Game/Design/Widgets/WBP_Viewport.WBP_LockerSkillCheck` (`self.Viewport`)) MovementInputs)
  (return false))

(fn `PressingLockerNow`
  (returns (FreeFromInteraction :type Boolean))
  (bind _isfreefrominteraction (`/Game/Design/Widgets/Interactions/WBP_LockerSkillCheck.ReceiveInteractionPress` (`/Game/Design/Widgets/WBP_Viewport.WBP_LockerSkillCheck` (`self.Viewport`))))
  (if _isfreefrominteraction
    (`self.ShowLockerSkillCheck` false)
    (`/EventDispatcherHub/FunctionLibrary/BPL_EventDispatcherHub.Call Single Gameplay Event` (struct :`TagName` "Event.Locker.Open") self)
    (return true)
    (else
      (return false))))

(fn `ReceiveEvent`
  (params (CalledTag :type "GameplayTag Structure") (CallingObject :type "Object Object Reference (by ref)"))
  (returns (Return :type Boolean))
  (return false))

(fn `SetNoUIMode`
  (params (ShouldHideUI :type Boolean))
  (returns (Return :type Boolean))
  (`Widget.SetVisibility` (`/Game/Design/Widgets/WBP_Viewport.GameCanvas` (`self.Viewport`)) (select `bool` ShouldHideUI :`false` "Visible" :`true` "Hidden" :!type "ESlateVisibility Enum"))
  (`KismetSystemLibrary.PrintString` "Hello")
  (return true))

(fn `ShowHideCheatMenuVisibility`
  (params (CheatManager :type "CheatManager Object Reference") (PlayerController :type "PlayerController Object Reference") (NewVisibility :type Boolean) (ShouldToggle :type Boolean))
  (returns (ResultVisibility :type Boolean))
  (bind _playercontroller (`local.PlayerController`))
  (`/Engine/EditorBlueprintResources/StandardMacros.IsValid` CheatManager
    (:`Is Valid`
      (if ShouldToggle
        (set `self.isCheatMenuVisible` (not (`self.isCheatMenuVisible`)))
        (else
          (set `self.isCheatMenuVisible` NewVisibility)))
      (if (`self.isCheatMenuVisible`)
        (bind _cheatmenu (`self.CheatMenu`)
          (:`then`
            (`/Game/Design/Widgets/CheatMenu/WBP_CheatMenu.ShowCheatMenu` _cheatmenu))
          (:`else`
            ;[0.4427 0.1807 0.3046 0.33] Push (create & set focus) CheatMenu
            (bind _returnvalue (`CommonActivatableWidgetContainerBase.BP_AddWidget` (`/Game/Design/Widgets/WBP_Viewport.CheatMenuSlot` (`self.Viewport`)) "/Game/Design/Widgets/CheatMenu/WBP_CheatMenu.WBP_CheatMenu_C"))
            (bind _output_get (set `self.CheatMenu` _returnvalue))
            (`/Game/Design/Widgets/CheatMenu/WBP_CheatMenu.Populate Cheats` _output_get (`local.CheatManager`))))
        (return (`self.isCheatMenuVisible`))
        (else
          (bind _cheatmenu_2 (`self.CheatMenu`)
            (:`then`
              (`/Game/Design/Widgets/CheatMenu/WBP_CheatMenu.HideCheatMenu` _cheatmenu_2)
              (`WidgetBlueprintLibrary.SetInputMode_GameOnly` _playercontroller)
              (set `PlayerController.bShowMouseCursor` false _playercontroller)
              (return (`self.isCheatMenuVisible`)))
            (:`else`)))))))

(fn `ShowLockerSkillCheck`
  (params (NewLockerVisibility :type Boolean))
  (returns (Return :type Boolean))
  (bind _wbp_lockerskillcheck (`/Game/Design/Widgets/WBP_Viewport.WBP_LockerSkillCheck` (`self.Viewport`)))
  (`Widget.SetVisibility` _wbp_lockerskillcheck (select `bool` NewLockerVisibility :`false` "Collapsed" :`true` "HitTestInvisible" :!type "ESlateVisibility Enum"))
  (if NewLockerVisibility
    (`/Game/Design/Widgets/Interactions/WBP_LockerSkillCheck.ShowUpFirstTime` _wbp_lockerskillcheck)
    (return true)
    (else
      (return true))))

(fn `ShowNewTextIndication`
  (params (IndicationToShow :type Text))
  (returns (Return :type Boolean))
  (`/Game/Design/Widgets/WBP_ScreenIndications.SetNewIndication` (`/Game/Design/Widgets/WBP_Viewport.WBP_ScreenIndications` (`self.Viewport`)) IndicationToShow)
  (return false))

(fn `UpdateAmmoCount`
  (returns (Return :type Boolean))
  (`/Game/Design/Widgets/ReloadSystem/WBP_ReloadSystem_QTE_MainUI.UpdateAmmoText` (`/Game/Design/Widgets/WBP_Viewport.WBP_ReloadSystem_QTE_MainUI` (`self.Viewport`)))
  (return true))

(fn `UpdatePrompts`
  (params (InteractionType :type "E_InteractionType Enum" :default "INTERACT"))
  (returns (Return :type Boolean))
  (`/Game/Design/Widgets/WBP_Viewport.UpdatePrompts` (`self.Viewport`) InteractionType)
  (return false))

(fn `UpdateReloadSystemState`
  (params (NewState :type "/Game/Design/ReloadSystem/Enums/E_PrimaryGunReloadState Enum" :default "NewEnumerator0"))
  (returns (Return :type Boolean))
  (`/Game/Design/Widgets/ReloadSystem/WBP_ReloadSystem_QTE_MainUI.OnReloadUpdated` (`/Game/Design/Widgets/WBP_Viewport.WBP_ReloadSystem_QTE_MainUI` (`self.Viewport`)) NewState)
  (return true))

(fn `UserConstructionScript`)