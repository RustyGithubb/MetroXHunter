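; Difficulty cheat function that switches the player's aim assist between Easy, Medium and disabled.
; On init it waits a tick, then caches the controlled pawn's aim assist component and the AimAssist cheat function from the cheat manager.
; OnCheat wraps Index over three states: Easy and Medium apply their settings, enable the component, initialize its HUD and sync the AimAssist cheat's Index.
; The third state delegates disabling to that cheat.
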(event `self.OnInit`
  (`KismetSystemLibrary.DelayUntilNextTick`)
  (`self.GetReferences`))

(event `self.OnCheat`
  (bind _aimassistcomponent (`self.AimAssistComponent`))
  (if (== (`self.Index`) 3)
    (set `self.Index` 0))
  (switch `int` (`self.Index`)
    (:`0`
      (`/AdvancedAimAssist/Blueprints/Components/AAA_BP_AimAssistComponent.UpdateAimAssistSettings` _aimassistcomponent "/Game/0_Design/GameDifficulty/Difficulty_Easy_AimAssist.Difficulty_Easy_AimAssist")
      (set `/AdvancedAimAssist/Blueprints/Components/AAA_BP_AimAssistComponent.bIsComponentEnable` true _aimassistcomponent :!label _label)
      (`/AdvancedAimAssist/Blueprints/Components/AAA_BP_AimAssistComponent.Initialize HUD` _aimassistcomponent)
      (set `MXHCheatSelectionFunction.Index` 1 (`self.AimAssistCheatFunction`)))
    (:`1`
      (`/AdvancedAimAssist/Blueprints/Components/AAA_BP_AimAssistComponent.UpdateAimAssistSettings` _aimassistcomponent "/Game/0_Design/GameDifficulty/Difficulty_Medium_AimAssist.Difficulty_Medium_AimAssist")
      (goto _label))
    (:`2`
      (`/Game/0_Design/CheatFunctions/BP_CheatFunction_AimAssist.DisableAimAssist` (`self.AimAssistCheatFunction`)))))

(fn `GetReferences`
  (set `self.AimAssistComponent` (`Actor.GetComponentByClass` (`Controller.K2_GetPawn` (`CheatManager.GetPlayerController` (`self.CheatManager`))) "/AdvancedAimAssist/Blueprints/Components/AAA_BP_AimAssistComponent.AAA_BP_AimAssistComponent_C"))
  (bind _returnvalue (`MXHCheatManager.FindCheatFunctionOfClass` (`self.CheatManager`) "/Game/0_Design/CheatFunctions/BP_CheatFunction_AimAssist.BP_CheatFunction_AimAssist_C"))
  (bind _asbp_cheat_function_aim_assist (cast `/Game/0_Design/CheatFunctions/BP_CheatFunction_AimAssist` _returnvalue))
  (set `self.AimAssistCheatFunction` _asbp_cheat_function_aim_assist))