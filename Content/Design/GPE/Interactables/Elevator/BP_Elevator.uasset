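; Interactable elevator that opens on interaction, then carries the player through a one-time ride with credits.
; Entering the trigger box freezes running; after delays it enables soft collision, plays the end door sequence and creates the credits widget.
; Tick then moves the mesh to a target point along a float curve under a looping camera animation with audio.
; When the curve ends, the camera animation stops and the open sequence replays.
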(event `self.InteractableComponent.OnInteract`
  ;[1 1 1 0.33] INTERACTION
  (`ActorSequenceComponent.PlaySequence` (`self.ActorSequence Open`))
  (`GameplayStatics.PlaySoundAtLocation` "/Game/Sounds/Audio/Ambient/Elevator/SW_Elevator.SW_Elevator" (`SceneComponent.K2_GetComponentLocation` (`self.RightDoor`)) (struct) 0.8 1.0 0.0 "/Game/Sounds/Attenuations/SA_Reverb.SA_Reverb" null null null)
  (`self.SetInteractionFreezed` true))

(event `self.TriggerBox.OnComponentBeginOverlap`
  (params (OverlappedComponent :type "PrimitiveComponent Object Reference") (OtherActor :type "Actor Object Reference") (OtherComp :type "PrimitiveComponent Object Reference") (OtherBodyIndex :type Integer) (bFromSweep :type Boolean) (SweepResult :type "HitResult Structure (by ref)"))
  ;[1 1 1 0.33] Comment
  (`/Game/Design/EnvironmentEvents/Components/BP_TriggerEventReceiver_Component.OnPlayComponentSpecificEvent` (`self.BP_SwitchData3CTriggerEventReceiver_Component`) true null)
  (bind _asmetro_player_controller (cast `MetroPlayerController` (`GameplayStatics.GetPlayerController` 0))
    (:`then`
      (`CharacterControllerComponent.ToggleFreezeRun` (`self.GetComponentByClass` _asmetro_player_controller "/Script/MetroXHunter.CharacterControllerComponent") true))
    (:`CastFailed`
      _))
  (`KismetSystemLibrary.Delay` 1.0)
  (if (not (`self.bIsTriggered`))
    ;[1 0 0 1 30] Lancement mise en scéne
    (`PrimitiveComponent.SetCollisionEnabled` (`self.Soft Collision`) "QueryAndPhysics")
    (set `self.bIsTriggered` true)
    (`KismetSystemLibrary.Delay` 1.0)
    (`ActorSequenceComponent.PlaySequence` (`self.ActorSequence End`))
    (`GameplayStatics.PlaySoundAtLocation` "/Game/Sounds/Audio/Ambient/Elevator/SW_Elevator_OpenDoor.SW_Elevator_OpenDoor" (`SceneComponent.K2_GetComponentLocation` (`self.RightDoor`)) (struct) 0.8 1.0 0.0 "/Game/Sounds/Attenuations/SA_Reverb.SA_Reverb" null null null)
    ;;[1 1 1 0.33] Temp animation Sequencer
    (`KismetSystemLibrary.Delay` 2.0)
    ;[0.01929 1 0 0.33] TO CHANGE
    (bind _returnvalue (`|CreateWidget` "/Game/Design/Widgets/Introduction/WBP_Credits.WBP_Credits_C"))
    (`UserWidget.AddToViewport` _returnvalue 0)
    (set `self.Initial Position` (`SceneComponent.K2_GetComponentLocation` (`self.StaticMesh`)))
    (set `self.Final Position` (`SceneComponent.K2_GetComponentLocation` (`self.Target Point`)))
    (`self.SetActorTickEnabled` true)
    (bind _returnvalue_2 (`CameraAnimationCameraModifier.PlayCameraAnimation` (`CameraAnimationCameraModifier.GetCameraAnimationCameraModifierFromPlayerController` (`GameplayStatics.GetPlayerController` 0)) (`self.Sequence`) (make `CameraAnimationParams` 1.0 1.0 "Sinusoidal" 1.5 "Sinusoidal" 1.5 true)))
    (`WidgetComponent.SetWidget` (`self.Widget`) null)
    (`AudioComponent.Play` (`self.Audio`) 0.0)))

(event `self.ReceiveTick`
  (params (DeltaSeconds :type "Float (single-precision)"))
  (bind _curve_locomotion (`self.curve locomotion`))
  ;[0 0 0] Timer
  (set `self.Timer Curve` (+ (`self.Timer Curve`) (`GameplayStatics.GetWorldDeltaSeconds`)))
  ;[0 0 0] Locomotion
  (`SceneComponent.K2_SetWorldLocation` (`self.StaticMesh`) (`KismetMathLibrary.VLerp` (`self.Initial Position`) (`self.Final Position`) (`CurveFloat.GetFloatValue` _curve_locomotion (`self.Timer Curve`))) false false)
  ;[1 0 0 1 20] Condition end animation
  (if (>= (`self.Timer Curve`) (`.MaxTime` (`CurveBase.GetTimeRange` _curve_locomotion)))
    (`self.SetActorTickEnabled` false)
    (`CameraAnimationCameraModifier.StopCameraAnimation` (`CameraAnimationCameraModifier.GetCameraAnimationCameraModifierFromPlayerController` (`GameplayStatics.GetPlayerController` 0)) (stale `self.TriggerBox.OnComponentBeginOverlap` _returnvalue_2) false)
    (`ActorSequenceComponent.PlaySequence` (`self.ActorSequence Open`))))

(event `self.TriggerBox.OnComponentEndOverlap`
  (params (OverlappedComponent :type "PrimitiveComponent Object Reference") (OtherActor :type "Actor Object Reference") (OtherComp :type "PrimitiveComponent Object Reference") (OtherBodyIndex :type Integer))
  ;[1 1 1 0.33] Comment
  (`/Game/Design/EnvironmentEvents/Components/BP_TriggerEventReceiver_Component.OnPlayComponentSpecificEvent` (`self.BP_SwitchData3CTriggerEventReceiver_Component`) false null)
  (bind _asmetro_player_controller (cast `MetroPlayerController` (`GameplayStatics.GetPlayerController` 0)))
  (`CharacterControllerComponent.ToggleFreezeRun` (`self.GetComponentByClass` _asmetro_player_controller "/Script/MetroXHunter.CharacterControllerComponent") false))

(fn `UserConstructionScript`)