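; AI target component that rations a limited token pool and ordered group places among actors that reserve them on its owner.
; Token requests succeed only while enough remain, tracked per reserver in a map.
; Reservers take the first group with space (zero means unlimited); freeing a limited place promotes an actor from the next group and notifies it by message.
; Tick, enabled by a debug flag, draws token usage above the owner.
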(event `self.ReceiveBeginPlay`
  (`self.ResetTokens`)
  (`self.SetComponentTickEnabled` (`self.IsDrawDebugEnabled`)))

(event `self.ReceiveTick`
  (params (DeltaSeconds :type "Float (single-precision)"))
  (`KismetSystemLibrary.DrawDebugString` (+ (`Actor.K2_GetActorLocation` (`self.GetOwner`)) (0.0 0.0 75.0)) (`KismetTextLibrary.Conv_TextToString` (`|FormatText` "[AITargetComponent] \nTokens: {RemainingTokens}/{MaxTokens} \nReservations: \n{Reservations}" (`self.GetRemainingTokens`) (`self.MaxTokens`) (`self.FormatReservedTokens`))) null))

(fn `FormatReservedTokens`
  (returns (Text :type String))
  (locals (FormattedText :type String))
  (bind _reservedtokens (`self.ReservedTokens`))
  (bind _keys (`BlueprintMapLibrary.Map_Keys` _reservedtokens))
  (for _array_element _keys
    (set `local.FormattedText` (`KismetStringLibrary.Concat_StrStr` (`local.FormattedText`) (`KismetTextLibrary.Conv_TextToString` (`|FormatText` "- {Actor}: {Tokens} \n" _array_element (`BlueprintMapLibrary.Map_Find` _reservedtokens _array_element))))))
  (return (`local.FormattedText`)))

(fn `FreeAllTokens`
  (params (Reserver :type "Actor Object Reference"))
  (`BlueprintMapLibrary.Map_Remove` (`self.ReservedTokens`) Reserver))

(fn `FreeGroupPlace`
  (params (Reserver :type "Actor Object Reference"))
  (locals (GroupIndex :type Integer))
  (bind _reservedgroupplaces (`self.ReservedGroupPlaces`))
  (bind _groupindex (`local.GroupIndex`))
  (bind (_value _returnvalue) (`BlueprintMapLibrary.Map_Find` _reservedgroupplaces Reserver))
  (set `local.GroupIndex` _value)
  (if _returnvalue
    (`BlueprintMapLibrary.Map_Remove` _reservedgroupplaces Reserver)
    (if (and (> (`|GetArrayItem` (`self.MaxGroupsPlaces`) (`local.GroupIndex`)) 0) (< (`local.GroupIndex`) (- (`KismetArrayLibrary.Array_Length` (`self.MaxGroupsPlaces`)) 1)))
      (bind _actorsbygroupplaces (`self.GetActorsByGroupPlaces`)) ; NOTE: Probably too much for current implementation
      (`self.MoveGroupPlace` (`|GetArrayItem` (break `/Game/0_Design/F_ActorArray` (`BlueprintMapLibrary.Map_Find` _actorsbygroupplaces (+ _groupindex 1)))) _groupindex))))

(fn `FreeReservations`
  (params (Reserver :type "Actor Object Reference"))
  (`self.FreeAllTokens` Reserver)
  (`self.FreeGroupPlace` Reserver))

(fn `FreeTokens`
  (params (Reserver :type "Actor Object Reference") (Tokens :type Integer))
  (bind _reservedtokens (`self.ReservedTokens`))
  (`BlueprintMapLibrary.Map_Add` _reservedtokens Reserver (`KismetMathLibrary.Max` (- (`BlueprintMapLibrary.Map_Find` _reservedtokens Reserver) Tokens))))

(fn `GetActorsByGroupPlaces`
  (returns (ActorsByGroupPlaces :type "Map of Integer to /Game/0_Design/F_ActorArray Structure"))
  (locals (_ActorsByGroupPlaces :type "Map of Integer to /Game/0_Design/F_ActorArray Structure") (Array :type "Array of Actor Object Reference"))
  (bind __actorsbygroupplaces (`local._ActorsByGroupPlaces`))
  (bind _keys (`BlueprintMapLibrary.Map_Keys` (`self.ReservedGroupPlaces`)))
  (for _array_element _keys
    (bind _value (`BlueprintMapLibrary.Map_Find` (`self.ReservedGroupPlaces`) _array_element))
    (bind _output_get (set `local.Array` (break `/Game/0_Design/F_ActorArray` (`BlueprintMapLibrary.Map_Find` __actorsbygroupplaces _value))))
    (`KismetArrayLibrary.Array_Add` _output_get _array_element)
    (`BlueprintMapLibrary.Map_Add` __actorsbygroupplaces _value (make `/Game/0_Design/F_ActorArray` _output_get)))
  (return (`local._ActorsByGroupPlaces`)))

(fn `GetRemainingGroupPlaces`
  (params (GroupIndex :type Integer))
  (returns (Places :type Integer))
  (locals (Count :type Integer))
  (bind _values (`BlueprintMapLibrary.Map_Values` (`self.ReservedGroupPlaces`)))
  (for _array_element _values
    (if (== _array_element GroupIndex)
      (`/Engine/EditorBlueprintResources/StandardMacros.IncrementInt` (`local.Count`))))
  (return (- (`|GetArrayItem` (`self.MaxGroupsPlaces`) GroupIndex) (`local.Count`))))

(fn `GetRemainingTokens`
  (returns (Tokens :type Integer))
  (locals (RemainingTokens :type Integer))
  (bind _remainingtokens (`local.RemainingTokens`))
  (bind _reservedtokens (`self.ReservedTokens`))
  (set `local.RemainingTokens` (`self.MaxTokens`))
  (bind _keys (`BlueprintMapLibrary.Map_Keys` _reservedtokens))
  (for _array_element _keys
    (`/Game/o_Libraries/BPL_GeneralUtilities.Decrease Value Int` _remainingtokens (`BlueprintMapLibrary.Map_Find` _reservedtokens _array_element)))
  (return _remainingtokens))

(fn `MoveGroupPlace`
  (params (Reserver :type "Actor Object Reference") (ToGroupIndex :type Integer))
  (bind _reservedgroupplaces (`self.ReservedGroupPlaces`))
  (`BlueprintMapLibrary.Map_Remove` _reservedgroupplaces Reserver)
  (`BlueprintMapLibrary.Map_Add` _reservedgroupplaces Reserver ToGroupIndex)
  (message `/Game/0_Design/Enemies/AI/BPI_AITarget_GroupPlaceReserver.OnGroupPlaceUpdated` Reserver self ToGroupIndex))

(fn `ReserveGroupPlace`
  (params (Reserver :type "Actor Object Reference"))
  (returns (GroupIndex :type Integer))
  (locals (_GroupIndex :type Integer :default -1))
  (bind __groupindex (`local._GroupIndex`))
  (for (_array_element _array_index) (`self.MaxGroupsPlaces`)
    (if (== _array_element 0)
      (set `local._GroupIndex` _array_index)
      (break)
      (elif (> (`self.GetRemainingGroupPlaces` _array_index) 0)
        (set `local._GroupIndex` _array_index)
        (break))))
  (`BlueprintMapLibrary.Map_Add` (`self.ReservedGroupPlaces`) Reserver __groupindex)
  (return __groupindex))

(fn `ReserveTokens`
  (params (Reserver :type "Actor Object Reference") (Tokens :type Integer))
  (returns (bIsSuccess :type Boolean))
  (`/Engine/EditorBlueprintResources/StandardMacros.IsValid` Reserver
    (:`Is Valid`
      (if (>= (`self.GetRemainingTokens`) Tokens)
        (`BlueprintMapLibrary.Map_Add` (`self.ReservedTokens`) Reserver (`local.Tokens`))
        (return true)
        (else
          (return false))))
    (:`Is Not Valid`
      (return false))))

(fn `ResetTokens`
  (`BlueprintMapLibrary.Map_Clear` (`self.ReservedTokens`)))