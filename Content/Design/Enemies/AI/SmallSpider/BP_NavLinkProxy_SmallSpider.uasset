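; Nav link proxy that lets small spiders climb between points on the navmesh.
; When a BP_SmallSpider reaches the smart link, it calls ClimbTo on that spider's AI controller with the link destination.
; With AI debug enabled, it draws the destination and an L-shaped arrow path, going vertical first when climbing up and horizontal first otherwise.
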(event `self.ReceiveSmartLinkReached`
  (params (Agent :type "Actor Object Reference") (Destination :type "Vector Structure (by ref)"))
  (bind _z (.z Destination))
  (bind _returnvalue (`self.K2_GetActorLocation` Agent))
  (bind _z_2 (.z _returnvalue))
  (bind _returnvalue_2 (`KismetMathLibrary.SelectVector` (`KismetMathLibrary.MakeVector` (.x Destination) (.y Destination) _z_2) (`KismetMathLibrary.MakeVector` (.x _returnvalue) (.y _returnvalue) _z) (<= _z _z_2)))
  (bind _asbp_small_spider (cast `/Game/Design/Enemies/AI/SmallSpider/BP_SmallSpider` Agent))
  (bind _asbp_small_spider_aicontroller (cast `/Game/Design/Enemies/AI/SmallSpider/BP_SmallSpider_AIController` (`Pawn.GetController` _asbp_small_spider)))
  (`/Game/Design/Enemies/AI/SmallSpider/BP_SmallSpider_AIController.ClimbTo` _asbp_small_spider_aicontroller Destination)
  (if (`ConvarLibrary.IsAIDebugConvarEnabled`)
    (`KismetSystemLibrary.DrawDebugSphere` Destination 64.0 12 (struct :`R` 0.266667 :`B` 1.0 :`A` 1.0) 3.0 4.0)
    (`KismetSystemLibrary.DrawDebugArrow` _returnvalue _returnvalue_2 128.0 (struct :`R` 0.266667 :`B` 1.0 :`A` 1.0) 3.0 4.0)
    (`KismetSystemLibrary.DrawDebugArrow` _returnvalue_2 Destination 128.0 (struct :`R` 0.266667 :`B` 1.0 :`A` 1.0) 3.0 4.0)))

(fn `UserConstructionScript`)