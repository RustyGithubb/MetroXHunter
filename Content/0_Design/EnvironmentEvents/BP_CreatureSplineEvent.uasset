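; Environment event actor that moves a skeletal-mesh creature along a spline when a trigger box is entered.
; The mesh waits hidden at the first spline point until the trigger receiver component's enter event shows it and enables tick.
; Tick advances a timer to set mesh location and rotation along the spline, then hides it and stops ticking at the spline's duration.
; The timer is never reset here, and trigger exit does nothing.
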(event `self.ReceiveBeginPlay`
  (`SceneComponent.K2_SetRelativeLocation` (`self.SkeletalMeshComponent`) (`SplineComponent.GetLocationAtSplinePoint` (`self.Spline`) 0 "Local") false false)
  (`SceneComponent.SetVisibility` (`self.SkeletalMeshComponent`) false false)
  (`self.SetActorTickEnabled` false))

(event `self.ReceiveTick`
  (params (DeltaSeconds :type "Float (single-precision)"))
  (bind (_returnvalue_location _returnvalue_rotation) (`KismetMathLibrary.BreakTransform` (`SplineComponent.GetTransformAtTime` (`self.Spline`) (`self.CurrentMovementTimer`) "Local" false false)))
  (bind _return (`/Game/o_Libraries/BPL_GeneralUtilities.Increase Value Float` (`self.CurrentMovementTimer`) (`GameplayStatics.GetWorldDeltaSeconds`)))
  (if (>= _return (`SplineComponent.Duration` (`self.Spline`)))
    (`self.EndSplineMovement`)
    (else
      (`SceneComponent.K2_SetRelativeLocationAndRotation` (`self.SkeletalMeshComponent`) _returnvalue_location _returnvalue_rotation false false))))

(event `EndSplineMovement`
  (`SceneComponent.SetVisibility` (`self.SkeletalMeshComponent`) false false)
  (`self.SetActorTickEnabled` false))

(event `self.BP_TriggerEventReceiver_Component.OnTriggerBoxEnter`
  (`SceneComponent.SetVisibility` (`self.SkeletalMeshComponent`) true false)
  (`self.SetActorTickEnabled` true))

(event `self.BP_TriggerEventReceiver_Component.OnTriggerBoxExit`)

(fn `SpawnNewLinkedTriggerBox`
  (`/Game/0_Design/EnvironmentEvents/BP_TriggerEventReceiver_Component.SpawnNewLinkedTriggerBox` (`self.BP_TriggerEventReceiver_Component`)))

(fn `UserConstructionScript`)