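; Cheat function that switches the player's aim assist between Easy, Medium and disabled based on its Index, which wraps at 3.
; On init it waits a tick, then caches the pawn's AimAssistComponent and the AimAssist cheat function from the CheatManager.
; Easy and Medium apply their settings, enable the component, initialize its HUD and set the AimAssist cheat's Index to 1.
; The third state delegates disabling to that cheat.
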(event `self.OnInit`
  (`KismetSystemLibrary.DelayUntilNextTick`)
  (`self.GetReferences`))

(event `self.OnCheat`
  (bind _aimassistcomponent (`self.AimAssistComponent`))
  (if (== (`self.Index`) 3)
    (set `self.Index` 0))
  (switch `int` (`self.Index`)
    (:`0`
      (`/AdvancedAimAssist/Blueprints/Components/AAA_BP_AimAssistComponent.UpdateAimAssistSettings` _aimassistcomponent "/Game/Design/GameDifficulty/Difficulty_Easy_AimAssist.Difficulty_Easy_AimAssist")
      (set `/AdvancedAimAssist/Blueprints/Components/AAA_BP_AimAssistComponent.bIsComponentEnable` true _aimassistcomponent :!label _label)
      (`/AdvancedAimAssist/Blueprints/Components/AAA_BP_AimAssistComponent.Initialize HUD` _aimassistcomponent)
      (set `MetroCheatSelectionFunction.Index` 1 (`self.AimAssistCheatFunction`)))
    (:`1`
      (`/AdvancedAimAssist/Blueprints/Components/AAA_BP_AimAssistComponent.UpdateAimAssistSettings` _aimassistcomponent "/Game/Design/GameDifficulty/Difficulty_Medium_AimAssist.Difficulty_Medium_AimAssist")
      (goto _label))
    (:`2`
      (`/Game/Design/CheatFunctions/BP_CheatFunction_AimAssist.DisableAimAssist` (`self.AimAssistCheatFunction`)))))

(fn `GetReferences`
  (bind _returnvalue (`Controller.K2_GetPawn` (`CheatManager.GetPlayerController` (`self.CheatManager`))))
  (`/Engine/EditorBlueprintResources/StandardMacros.IsValid` _returnvalue
    (:`Is Valid`
      (set `self.AimAssistComponent` (`Actor.GetComponentByClass` _returnvalue "/AdvancedAimAssist/Blueprints/Components/AAA_BP_AimAssistComponent.AAA_BP_AimAssistComponent_C"))
      (bind _returnvalue_2 (`MetroCheatManager.FindCheatFunctionOfClass` (`self.CheatManager`) "/Game/Design/CheatFunctions/BP_CheatFunction_AimAssist.BP_CheatFunction_AimAssist_C"))
      (set `self.AimAssistCheatFunction` _returnvalue_2))))