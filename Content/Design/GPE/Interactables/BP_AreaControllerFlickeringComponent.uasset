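; Area controller component that manages a group of referenced actors' lights, tunnel lamps and circuit breakers.
; On BeginPlay it replaces the owner's tags with cinematic tags and caches a light component from each controlled actor.
; ShouldChangeType pushes a shared off-state to tunnel lamps and circuit breakers, then refreshes them.
; TakeDamageActualisationArea has the game mode's LightManagerComponent flicker the cached lights using a supplied curve and the player's location.
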(event `self.ReceiveBeginPlay`
  (set `Actor.Tags` (`self.Tags Cinematique`) (`self.GetOwner`))
  (for _array_element (`self.Actor to Control`)
    (bind _returnvalue (`Actor.GetComponentByClass` _array_element "/Script/Engine.LightComponent"))
    (`/Engine/EditorBlueprintResources/StandardMacros.IsValid` _returnvalue
      (:`Is Valid`
        (`KismetArrayLibrary.Array_Add` (`self.Lights`) _returnvalue)))))

(event `Should Change Type`
  (bind _should_off_change_value (`self.Should OFF Change Value`))
  (for _array_element (`self.Actor to Control`)
    (bind _asbp_tunnel_lamp (cast `/Game/Art/0_Mesh/GPE/BP_TunnelLamp` _array_element))
    (set `/Game/Art/0_Mesh/GPE/BP_TunnelLamp.Should OFF` _should_off_change_value _asbp_tunnel_lamp)
    (`/Game/Art/0_Mesh/GPE/BP_TunnelLamp.After Be referenced` _asbp_tunnel_lamp))
  (for _array_element_2 (`self.Actor to Control`)
    (bind _asbp_circuit_breaker (cast `/Game/Design/GPE/Interactables/BP_CircuitBreaker` _array_element_2))
    (set `/Game/Design/GPE/Interactables/BP_CircuitBreaker.Should OFF` _should_off_change_value _asbp_circuit_breaker)
    (`/Game/Design/GPE/Interactables/BP_CircuitBreaker.ReFresh State` _asbp_circuit_breaker)))

(event `Take Damage Actualisation Area`
  (params (FlickeringLightCurve :type "CurveVector Object Reference"))
  (`LightManagerComponent.FlickerLightsInArray` (`Actor.GetComponentByClass` (`GameplayStatics.GetGameMode`) "/Script/MetroXHunter.LightManagerComponent") (`self.Lights`) (`Actor.K2_GetActorLocation` (`GameplayStatics.GetPlayerCharacter` 0)) FlickeringLightCurve)
  (`KismetSystemLibrary.PrintString` "Hello"))