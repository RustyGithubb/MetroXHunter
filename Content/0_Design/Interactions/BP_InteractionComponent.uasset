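; Interaction component that tracks a list of interactables, triggers them on interact input and drives the on-screen prompt.
; Add and remove functions maintain a unique list, then refresh the viewport widget through player 0's BPC_Controller.
; Pressing IA_TPS_Interact calls CallOnInteract on every listed item, rather than a single chosen target.
; The prompt update runs once per item with its interaction type, or uses the default when the list is empty.
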(event `EnhancedInput|/TPS_FeedlingAddon/TPS/_Input/IA_TPS_Interact`
  (params (ActionValue :type Boolean) (ElapsedSeconds :type "Float (double-precision)") (TriggeredSeconds :type "Float (double-precision)") (InputAction :type "InputAction Object Reference" :default "/TPS_FeedlingAddon/TPS/_Input/IA_TPS_Interact.IA_TPS_Interact"))
  (:`Started`
    (for _array_element (`self.Interactables`)
      (`/Game/0_Design/Interactions/BP_InteractableComponent.OnInteract` _array_element))))

(fn `AddToInteractables`
  (params (Interactable :type "/Game/0_Design/Interactions/BP_InteractableComponent Object Reference (by ref)"))
  (`KismetArrayLibrary.Array_AddUnique` (`self.Interactables`) Interactable)
  (`self.UpdapteViewport`))

(fn `RemoveFromInteractables`
  (params (Item :type "/Game/0_Design/Interactions/BP_InteractableComponent Object Reference (by ref)"))
  (`KismetArrayLibrary.Array_RemoveItem` (`self.Interactables`) Item)
  (`self.UpdapteViewport`))

(fn `UpdapteViewport`
  (if (> (`KismetArrayLibrary.Array_Length` (`self.Interactables`)) 0)
    (for _array_element (`self.Interactables`)
      (bind _asbpc_controller (cast `/Game/0_Design/GameManagement_/BPC_Controller` (`GameplayStatics.GetPlayerController` 0)))
      (`/Game/UI/Widgets/WBP_Viewport.UpdatePrompts` (`/Game/0_Design/GameManagement_/BPC_Controller.ViewportWidget` _asbpc_controller) (`/Game/0_Design/Interactions/BP_InteractableComponent.InteractionType` _array_element)))
    (else
      (bind _asbpc_controller_2 (cast `/Game/0_Design/GameManagement_/BPC_Controller` (`GameplayStatics.GetPlayerController` 0)))
      (`/Game/UI/Widgets/WBP_Viewport.UpdatePrompts` (`/Game/0_Design/GameManagement_/BPC_Controller.ViewportWidget` _asbpc_controller_2) "DEFAULT"))))