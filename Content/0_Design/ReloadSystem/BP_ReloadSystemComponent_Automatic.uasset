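; Reload system component for a gun that automatically refills its magazine over time, driven by an on-screen widget.
; Firing notifies the widget and starts refilling, which advances every Tick by RefillSpeed without delta-time scaling until the widget reports a full magazine.
; Each widget reload event adds one round to the gun.
; Reload input instantly fills the magazine; its commented reload-item check is hardcoded true.
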(event `self.ReceiveBeginPlay`
  (bind _widget (`self.Widget`))
  (bind _gun (`self.Gun`))
  (`self.CreateWidget`)
  (add `/Game/0_Design/GameManagement_/BP_Gun.OnFire` (`self.Gun`) (delegate `OnFire`))
  (add `/Game/UI/Widgets/WBP_ReloadSystem_Automatic.OnMagazineRefilled` _widget (delegate `OnMagazineRefilled`))
  (add `/Game/UI/Widgets/WBP_ReloadSystem_Automatic.OnReload` _widget (delegate `OnReload`))
  (set `/Game/0_Design/GameManagement_/BP_Gun.IndexMagazineAmmo` (`/Game/0_Design/GameManagement_/BP_Gun.MaxMagazineAmmo` _gun) _gun))

(event `OnFire`
  (`/Game/UI/Widgets/WBP_ReloadSystem_Automatic.OnFire` (`self.Widget`))
  (set `self.IsMagazineFull` false))

(event `OnMagazineRefilled`
  (set `self.IsMagazineFull` true))

(event `OnReload`
  (`/Engine/EditorBlueprintResources/StandardMacros.IncrementInt` (`/Game/0_Design/GameManagement_/BP_Gun.IndexMagazineAmmo` (`self.Gun`))))

(event `self.ReceiveTick`
  (params (DeltaSeconds :type "Float (single-precision)"))
  (if (not (`self.IsMagazineFull`))
    (`/Game/UI/Widgets/WBP_ReloadSystem_Automatic.RefillBullet` (`self.Widget`) (/ (`self.RefillSpeed`) 100.0))))

(event `self.ReceiveEndPlay`
  (params (EndPlayReason :type "EEndPlayReason Enum" :default "Destroyed"))
  (`Widget.RemoveFromParent` (`self.Widget`)))

(fn `CreateWidget`
  (bind _asbpc_controller (cast `/Game/0_Design/GameManagement_/BPC_Controller` (`Pawn.GetController` (`self.PlayerCharacter`))))
  (bind _returnvalue (`|CreateWidget` "/Game/UI/Widgets/WBP_ReloadSystem_Automatic.WBP_ReloadSystem_Automatic_C" _asbpc_controller))
  (bind _output_get (set `self.Widget` _returnvalue))
  (set `/Game/UI/Widgets/WBP_ReloadSystem_Automatic.Drain Amount` (`self.Drain Amount`) _output_get)
  (set `/Game/UI/Widgets/WBP_ReloadSystem_Automatic.Block Amount` (`self.Block Amount`) _output_get)
  (`UserWidget.AddToViewport` _output_get 0))

(fn `OnReloadInput`
  (params (`Input Type` :type "/Game/0_Design/E_InputActionType Enum" :default "NewEnumerator0"))
  (bind _gun (`self.Gun`))
  (switch `/Game/0_Design/E_InputActionType` `Input Type`
    (:`NewEnumerator1`
      ;[1 1 1 0.33] If reload item
      (if true
        (set `/Game/0_Design/GameManagement_/BP_Gun.IndexMagazineAmmo` (`/Game/0_Design/GameManagement_/BP_Gun.MaxMagazineAmmo` _gun) _gun)
        (`/Game/UI/Widgets/WBP_ReloadSystem_Automatic.Reload` (`self.Widget`))))))