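; Spider enemy for the shooting range that moves toward the player via AI MoveTo and dies on reaching them.
; While running, it launches itself straight up once within jump range.
; Targeting swaps its material to an alpha variant and enables its weak points with the player's camera; untargeting reverts both.
; Any weak point's death signals the spider's death and destroys it.
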(event `self.ReceiveTick`
  (params (DeltaSeconds :type "Float (single-precision)"))
  ;[1 0 0.005598 0.25] TICK
  ;;[1 1 1 0.33] Jump to Target
  (if (and (`self.bIsRunning`) (not (`self.bIsJumping`)))
    (if (<= (`self.GetDistanceTo` (`self.Target`) self) (`self.JumpRange`))
      (`self.LaunchCharacter` (0.0 0.0 500.0))
      (set `self.bIsJumping` true))))

(event `self.ReceiveBeginPlay`
  ;[1 0 0.005598 0.25] BEGIN PLAY
  (`parent.ReceiveBeginPlay`)
  ;;[1 1 1 0.33] Bind WeakPoint's LifeComponent Event OnDeath
  (for _array_element (`self.WeakPoints`)
    (add `/Game/0_Design/LifeSystem/BP_LifeComponent.OnDeath` (`/Game/0_Design/EyeVisionSystem/BP_WeakPoints.LifeComponent` _array_element) (delegate `OnWeakPointDown`))
    (bind _output_get (set `self.Target` (`GameplayStatics.GetPlayerPawn` 0)))
    (`|AIMoveTo` self (0.0 0.0 0.0) _output_get
      (:`OnSuccess`
        (`self.OnDeath`)
        (`self.K2_DestroyActor`)))))

(event `OnWeakPointDown`
  ;[1 0 0.005598 0.25] BEGIN PLAY
  (`self.OnDeath`)
  (`self.K2_DestroyActor`))

(event `self.OnTargeted`
  (params (IsTargeted :type Boolean) (PlayerCamera :type "CineCameraComponent Object Reference"))
  (bind _mesh (`self.Mesh`))
  ;[1 0 0.005598 0.25] ON TARGETED
  (if IsTargeted
    (`PrimitiveComponent.SetMaterial` _mesh 0 "/Game/9_ShootingRange/Materials/MI_FlatColor_Alpha_Brown.MI_FlatColor_Alpha_Brown")
    ;;[1 1 1 0.33] Enable WeakPoints
    (for _array_element (`self.WeakPoints`)
      (`/Game/0_Design/EyeVisionSystem/BP_WeakPoints.EnableWeakPoint` _array_element PlayerCamera))
    (else
      (`PrimitiveComponent.SetMaterial` _mesh 0 "/Game/9_ShootingRange/Materials/MI_FlatColor_Brown.MI_FlatColor_Brown")
      ;;[1 1 1 0.33] Disable WeakPoints
      (for _array_element_2 (`self.WeakPoints`)
        (`/Game/0_Design/EyeVisionSystem/BP_WeakPoints.DisableWeakPoint` _array_element_2)))))

(fn `UserConstructionScript`
  (`parent.UserConstructionScript`))