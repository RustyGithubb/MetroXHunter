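; Environment-event receiver component that plays a configured sound when its component-specific event fires.
; It overrides OnPlayComponentSpecificEvent and, if the sound is valid, plays it either as 2D or at a set location with attenuation, based on a flag.
; Both paths share volume, pitch and start time settings and pass the component's owner as owning actor.
; The box-enter argument does not affect playback.
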(fn `OnPlayComponentSpecificEvent`
  (params (FromBoxEnter :type Boolean))
  (bind _soundstoplay (`self.SoundsToPlay`)
    (:`then`
      (if (`self.PlaySound2D`)
        (`GameplayStatics.PlaySound2D` _soundstoplay (`self.Volume Multiplier`) (`self.Pitch Multiplier`) (`self.Start Time`) null (`self.GetOwner`))
        (else
          (`GameplayStatics.PlaySoundAtLocation` _soundstoplay (`self.PlayLocation`) (struct) (`self.Volume Multiplier`) (`self.Pitch Multiplier`) (`self.Start Time`) (`self.Attenuation Settings`) null (`self.GetOwner`) null))))
    (:`else`)))