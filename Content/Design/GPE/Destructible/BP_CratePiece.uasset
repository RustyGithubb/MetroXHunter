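; BP_CratePiece is a short-lived debris piece, apparently for a destructible crate, that gets flung out and then disappears.
; BeginPlay sets a random lifespan, picks a random starting scale and applies a random-strength impulse to the static mesh along ImpulseDirection.
; Tick uses the remaining lifespan as a scale multiplier during the final second, shrinking the piece smoothly until it is destroyed.
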(event `self.ReceiveBeginPlay`
  (bind _lifetimerange (`self.LifetimeRange`))
  (bind _impulsestrengthrange (`self.ImpulseStrengthRange`))
  (`self.SetLifeSpan` (`KismetMathLibrary.RandomFloatInRange` (`.Value` (break `FloatRangeBound` (break `FloatRange` _lifetimerange))) (`.Value` (break `FloatRangeBound` (`.UpperBound` (break `FloatRange` _lifetimerange))))))
  (bind _output_get (set `self.StartingScale` (`KismetArrayLibrary.Array_Random` (`self.PossibleStartingScales`))))
  (`self.SetActorScale3D` _output_get)
  (`PrimitiveComponent.AddImpulse` (`self.StaticMeshComponent`) (* (`self.ImpulseDirection`) (`KismetMathLibrary.RandomFloatInRange` (`.Value` (break `FloatRangeBound` (break `FloatRange` _impulsestrengthrange))) (`.Value` (break `FloatRangeBound` (`.UpperBound` (break `FloatRange` _impulsestrengthrange)))))) "None" false))

(event `self.ReceiveTick`
  (params (DeltaSeconds :type "Float (single-precision)"))
  ;[1 1 1 0.33] if in the last second, get smaller before destroying
  (if (<= (`self.GetLifeSpan`) 1.0)
    (`self.SetActorScale3D` (* (`self.StartingScale`) (`self.GetLifeSpan`)))))

(fn `UserConstructionScript`)