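; Smart rat enemy that wanders on its own and can be killed, leaving blood and granting the RATATOUILLE_2 achievement.
; Tick turns it toward a random reachable point, re-picked every few seconds, while driving forward movement and a velocity-based material parameter.
; Its audio replays after random pauses.
; Death checks cached achievements, unlocks METRO when the GameInstance count completes, and destroys the actor only if RATATOUILLE_2 is already or successfully unlocked.
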(event `self.Health.OnDeath`
  (params (DamageContext :type "DamageContext Structure (by ref)"))
  (bind _returnvalue (`self.K2_GetActorLocation`))
  (bind _returnvalue_2 (`GameplayStatics.GetPlayerController` 0))
  (bind _returnvalue_3 (`GameplayStatics.GetPlayerController` 0))
  (bind _game_instance (`self.Game Instance`))
  ;[1 0 0 0.33] DESTROY
  (`GameplayStatics.SpawnDecalAtLocation` (`KismetArrayLibrary.Array_Random` (`|MakeArray` "/Game/Art/VFX/Materials/Blood/Puddles/MI_BloodPuddle_01.MI_BloodPuddle_01" "/Game/Art/VFX/Materials/Blood/Puddles/MI_BloodPuddle_02.MI_BloodPuddle_02" "/Game/Art/VFX/Materials/Blood/Puddles/MI_BloodPuddle_04.MI_BloodPuddle_04" :!type "MaterialInterface Object Reference")) (10.0 20.0 20.0) (- _returnvalue (0.0 0.0 10.0)))
  (`NiagaraFunctionLibrary.SpawnSystemAtLocation` "/Game/Art/VFX/NS_Blood/NS_Blood_Impact_Bullet.NS_Blood_Impact_Bullet" _returnvalue (struct) (0.2 0.2 0.2))
  ;[0 1 0.8336 0.33] ACHIEVEMENT : RATATOUILLE_2
  (`AchievementQueryCallbackProxy.CacheAchievements` _returnvalue_2
    (:`OnSuccess`
      (bind (_bfoundid _progress) (`AchievementBlueprintLibrary.GetCachedAchievementProgress` _returnvalue_2 "RATATOUILLE_2"))
      (if _bfoundid
        (if (> _progress 0.0)
          (`KismetSystemLibrary.PrintString` "Achievements already unlocked !" true true (struct :`G` 1.0 :`B` 0.012183 :`A` 1.0) 6.0)
          (`self.K2_DestroyActor` :!label _label)
          (else
            (`AchievementWriteCallbackProxy.WriteAchievementProgress` _returnvalue_2 "RATATOUILLE_2"
              (:`OnSuccess`
                (`|ExecutionSequence`
                  (:`then_0`
                    (goto _label))
                  (:`then_1`
                    (`KismetSystemLibrary.PrintString` "Achievement unlocked !" true true (struct :`G` 1.0 :`B` 0.96591 :`A` 1.0) 6.0)
                    (set `/Game/Design/_GameManagement/Core/BP_MetroGameInstance.AchievementsUnlocked` (+ (`/Game/Design/_GameManagement/Core/BP_MetroGameInstance.AchievementsUnlocked` _game_instance) 1) _game_instance)
                    (if (== (`/Game/Design/_GameManagement/Core/BP_MetroGameInstance.AchievementsUnlocked` _game_instance) (`/Game/Design/_GameManagement/Core/BP_MetroGameInstance.TotalNormalAchievements` _game_instance))
                      (bind (_bfoundid_2 _progress_2) (`AchievementBlueprintLibrary.GetCachedAchievementProgress` _returnvalue_3 "METRO"))
                      (if _bfoundid_2
                        (if (> _progress_2 0.0)
                          (`KismetSystemLibrary.PrintString` "Achievements already unlocked !" true true (struct :`G` 1.0 :`B` 0.012183 :`A` 1.0) 10.0)
                          (else
                            (`AchievementWriteCallbackProxy.WriteAchievementProgress` _returnvalue_3 "METRO")))
                        (else
                          (`KismetSystemLibrary.PrintString` "Didn't find ID" true true (struct :`R` 1.0 :`G` 0.408724 :`A` 1.0) 10.0))))))))))
        (else
          (`KismetSystemLibrary.PrintString` "Didn't find ID" true true (struct :`R` 1.0 :`G` 0.408724 :`A` 1.0) 6.0))))
    (:`OnFailure`
      (`KismetSystemLibrary.PrintString` "Couldn't cache achievements !" true true (struct :`R` 1.0 :`A` 1.0) 6.0))))

(event `self.ReceiveBeginPlay`
  (bind _staticmesh (`self.StaticMesh`))
  ;[1 0 0 0.33] BEGIN PLAY
  (`|ExecutionSequence`
    (:`then_0`
      (bind _returnvalue (`PrimitiveComponent.CreateDynamicMaterialInstance` _staticmesh 0 (`PrimitiveComponent.GetMaterial` _staticmesh 0) "None"))
      (set `self.Mat` _returnvalue)
      (add `AudioComponent.OnAudioFinished` (`self.Audio`) (delegate `OnAudioFinished`)))
    (:`then_1`
      (set `self.Current` (`self.GetActorForwardVector`)))
    (:`then_2`
      (bind _asbp_metro_game_instance (cast `/Game/Design/_GameManagement/Core/BP_MetroGameInstance` (`GameplayStatics.GetGameInstance`)))
      (set `self.Game Instance` _asbp_metro_game_instance))))

(event `OnAudioFinished`
  ;[1 0 0 0.33] BEGIN PLAY
  (`KismetSystemLibrary.Delay` (`KismetMathLibrary.RandomFloatInRange` 0.5 3.0))
  (`AudioComponent.Play` (`self.Audio`) 0.0))

(event `self.ReceiveTick`
  (params (DeltaSeconds :type "Float (single-precision)"))
  ;[1 1 1 0.33] EVENT TICK
  (set `self.Time Duration` (+ (`self.Time Duration`) DeltaSeconds))
  (`MaterialInstanceDynamic.SetScalarParameterValue` (`self.Mat`) "Velocity" (* (`KismetMathLibrary.VSize` (`self.GetVelocity`)) 2.0))
  ;[1 0.005787 0 1 30] RATS WANDER
  (`|ExecutionSequence`
    (:`then_0`
      (`self.K2_SetActorRotation` (`KismetMathLibrary.RInterpTo` (`self.K2_GetActorRotation`) (`KismetMathLibrary.FindLookAtRotation` (`self.K2_GetActorLocation` self) (`self.Direction To Look At`)) (`GameplayStatics.GetWorldDeltaSeconds`) 0.5))
      (`self.AddMovementInput` (`self.GetActorForwardVector`)))
    (:`then_1`
      (`KismetSystemLibrary.Delay` 3.0)
      (set `self.Direction To Look At` (`NavigationSystemV1.K2_GetRandomReachablePointInRadius` (`self.K2_GetActorLocation`) 500.0 null null)))))

(fn `GetEQSStartLocation`
  (returns (ReturnValue :type "Vector Structure"))
  (return (`self.K2_GetActorLocation`)))

(fn `GetEQSTargetActor`
  (returns (ReturnValue :type "Actor Object Reference"))
  (return null))

(fn `UserConstructionScript`)