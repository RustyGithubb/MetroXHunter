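; Aim assist component that, while the player aims, helps the crosshair and shots find nearby enemies.
; Each tick a sphere trace from screen center picks the target closest on screen and scales three zone radii by its distance.
; The magnetic zone slows the camera, the snap zone pulls rotation, and the bend zone redirects shot direction.
; Near-zero input starts a timer that switches assist off; an optional debug HUD shows zones and state.
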(event `self.ReceiveTick`
  (params (DeltaSeconds :type "Float (single-precision)"))
  ;[1 1 1 0.33] Check if Player is Aiming
  (if (`self.bIsPlayerAiming`)
    (`|ExecutionSequence`
      (:`then_0`
        ;[1 1 1 0.33] Check if Aim Assist is enable
        (if (`self.bIsAssistEnable`)
          ;[1 1 1 0.33] Find closest hit
          (bind (_hit_ _hitscreenlocation) (`self.Enemy Detection`))
          (`|ExecutionSequence`
            (:`then_0`
              ;[1 1 1 0.33] Check if there is a hit
              (if _hit_
                ;[1 1 1 0.33] Adjust CrossHair
                (bind _adjustedcrosshair (`self.AdjustPlayerAim` _hitscreenlocation))
                (set `self.AdjustCrossHairLocatin` _adjustedcrosshair)
                (else
                  ;[1 1 1 0.33] Reset Camera
                  (`self.ResetCamera`))))
            (:`then_1`
              ;[1 1 1 0.33] Update Debug AimAssist HUD
              (`self.UpdateHUD`)))))
      (:`then_1`
        (if (`self.bTriggerLowVelocity`)
          (`self.UpdateLockState` DeltaSeconds))))))

(fn `AdjustCircles`
  (params (CurrentTarget :type "Vector Structure"))
  (locals (DistanceRatio :type "Float (double-precision)"))
  (set `local.DistanceRatio` (- 1.0 (/ (`KismetMathLibrary.Vector_Distance` CurrentTarget (`Actor.K2_GetActorLocation` (`Controller.K2_GetPawn` (`self.PlayerController`)))) (`self.SphereTraceRange`))))
  (`|ExecutionSequence`
    (:`then_0`
      (set `self.AdjustedSZ` (* (`self.SnapZoneRadius`) (`local.DistanceRatio`))))
    (:`then_1`
      (set `self.AdjustedBZ` (* (`self.BendZoneRadius`) (`local.DistanceRatio`))))
    (:`then_2`
      (set `self.AdjustedMZ` (* (`self.MagneticZoneRadius`) (`local.DistanceRatio`))))
    (:`then_3`
      (if (`self.bIsDebugActivated`)
        (`/Game/External/AimAssit/Debug/HUD_AimAssist.OnCircleUpdate` (`self.AimAssistHUD`) (`|MakeArray` (`self.AdjustedBZ`) (`self.AdjustedSZ`) (`self.AdjustedMZ`)))))))

(fn `AdjustImpactPoint`
  (returns (ImpactDirection :type "Vector Structure"))
  (if (`self.bShouldAdjustImpact`)
    ;[0 0.2748 1 0.33] Return Screen Center to Closest Impact Point from target in world
    (return (`.WorldDirection` (`GameplayStatics.DeprojectScreenToWorld` (`self.PlayerController`) (`self.ClosestImpactPoint`))))
    (else
      ;[1 1 1 0.33] Return Screen Center to world impact
      (return (`.WorldDirection` (`GameplayStatics.DeprojectScreenToWorld` (`self.PlayerController`) (`self.ScreenCenter`)))))))

(fn `AdjustPlayerAim`
  (params (ClosestEnemyLocation :type "Vector2D Structure"))
  (returns (AdjustedCrossHair :type "Vector2D Structure"))
  (bind _distancefromcenter (`self.DistanceFromCenter`))
  ;[1 1 1 0.33] Get distance from center of screen
  ;[1 1 1 0.33] Check if in the Magnetic Zone
  (bind _output_get (set `self.DistanceFromCenter` (`KismetMathLibrary.Distance2D` ClosestEnemyLocation (`self.ScreenCenter`))))
  (if (< _output_get (`self.AdjustedMZ`))
    (`|ExecutionSequence`
      (:`then_0`
        ;[0.946 1 0 0.25] Camera Snap
        ;;[1 1 1 0.33] Check if target is Aligned with rotation
        (if (> (`KismetMathLibrary.DotProduct2D` (`self.InputDirectionNormalized`) (`KismetMathLibrary.Normal2D` (- (`local.ClosestEnemyLocation`) (`self.ScreenCenter`)))) (`self.Accuracy`))
          ;;[1 1 1 0.33] Check if in the Snap Zone
          (if (< _distancefromcenter (`self.AdjustedSZ`))
            ;;[1 1 1 0.33] Slow Camera Speed and adjust rotation
            (set `self.AimAssistMultiplier` (* 0.2 (`self.CameraSpeedMultiplier`)))
            (`self.AdjustPlayerRotation` (`local.ClosestEnemyLocation`) _distancefromcenter)
            (set `self.Assist State` "SNAP")
            (set `self.Color Current State` (struct :`R` 0.027451 :`G` 1.0 :`A` 1.0))
            (else
              ;;[1 1 1 0.33] Slow Down Camera Speed, depending on how close from the target is the crosshair
              (set `self.AimAssistMultiplier` (* (/ (`self.DistanceFromCenter`) (`self.AdjustedMZ`)) (`self.CameraSpeedMultiplier`)))
              (set `self.Assist State` "SLOW DOWN")
              (set `self.Color Current State` (struct :`R` 1.0 :`B` 0.67451 :`A` 1.0))))
          (else
            ;;[1 1 1 0.33] Reset Camera Speed
            (set `self.AimAssistMultiplier` 1.0))))
      (:`then_1`
        ;[0 0.2091 1 0.25] Bullet Magnetism
        ;;[1 1 1 0.33] Check if the feature is enable
        (if (`self.bEnableAdjustImpactPoint`)
          ;;[1 1 1 0.33] Check if within the Bend Zone radius
          (if (< (`KismetMathLibrary.Distance2D` (`self.ClosestImpactPoint`) (`self.ScreenCenter`)) (`self.AdjustedBZ`))
            (if (or (not (`self.bTriggerLowVelocity`)) (<= (`self.LowVelocityTimer`) 0.5))
              (set `self.bShouldAdjustImpact` true))
            (else
              (set `self.bShouldAdjustImpact` false)))))
      (:`then_2`
        ;[1 1 1 0.33] Return Closest Enemy Location
        (return (`local.ClosestEnemyLocation`))))
    (else
      ;[1 1 1 0.33] Return Screen Center Location
      (return (`self.ScreenCenter`)))))

(fn `AdjustPlayerRotation`
  (params (TargetHit :type "Vector2D Structure") (Distance :type "Float (double-precision)"))
  (bind _playercontroller (`self.PlayerController`))
  (bind (_x _y) (`KismetMathLibrary.BreakVector2D` (* (`KismetMathLibrary.Normal2D` (- TargetHit (`self.ScreenCenter`))) (* (/ Distance (`self.AdjustedSZ`)) (`self.MagneticForce`)))))
  ;[1 1 1 0.33] Apply Force to Yaw and Pitch inputs
  (`|ExecutionSequence`
    (:`then_0`
      (`PlayerController.AddYawInput` _playercontroller _x))
    (:`then_1`
      (`PlayerController.AddPitchInput` _playercontroller _y))))

(fn `Enemy Detection`
  (returns (`Hit?` :type Boolean) (HitScreenLocation :type "Vector2D Structure"))
  (locals (ClosestDistance :type "Float (double-precision)" :default 999.0) (HitToScreen :type "Vector2D Structure") (ClosestHit :type "HitResult Structure"))
  (bind _returnvalue (`WidgetLayoutLibrary.GetViewportSize`))
  (bind (_start _end) (`self.GetSphereTracePoints`))
  (bind (_bblockinghit _binitialoverlap _time _distance _location _impactpoint _normal _impactnormal _physmat _hitactor _hitcomponent) (`GameplayStatics.BreakHitResult` (`local.ClosestHit`)))
  (set `self.InputDirectionNormalized` (`KismetMathLibrary.Normal2D` (`self.Input Direction`)))
  ;[1 1 1 0.33] Set the ScreenSize of the HUD
  (bind _aimassisthud (`self.AimAssistHUD`)
    (:`then`
      (set `/Game/External/AimAssit/Debug/HUD_AimAssist.ScreenSize` _returnvalue _aimassisthud))
    (:`else`
      _))
  ;[1 1 1 0.33] Set Screen Center
  (set `self.ScreenCenter` (* _returnvalue 0.5))
  ;[1 1 1 0.33] Check if Monsters near crossHair
  (bind (_outhits _returnvalue_2) (`KismetSystemLibrary.SphereTraceMultiForObjects` _start _end (`self.SphereTraceRadius`) (`|MakeArray` "ObjectTypeQuery7" :!type "EObjectTypeQuery Enum")))
  (if _returnvalue_2
    (for _array_element _outhits
      (bind (_bblockinghit_2 _binitialoverlap_2 _time_2 _distance_2 _location_2 _impactpoint_2 _normal_2 _impactnormal_2 _physmat_2 _hitactor_2 _hitcomponent_2) (`GameplayStatics.BreakHitResult` _array_element))
      (bind _screenposition (`GameplayStatics.ProjectWorldToScreen` (`self.PlayerController`) _impactpoint_2))
      (bind _returnvalue_3 (`KismetMathLibrary.Distance2D` (`self.ScreenCenter`) _screenposition))
      ;[1 1 1 0.33] Check Closest hit from Crosshair (center of screen)
      (if (< _returnvalue_3 (`local.ClosestDistance`))
        (set `local.ClosestDistance` _returnvalue_3)
        ;[1 1 1 0.33] Update closest Hit Position
        (set `local.HitToScreen` (`GameplayStatics.ProjectWorldToScreen` (`self.PlayerController`) (`KismetSystemLibrary.GetComponentBounds` _hitcomponent_2)))
        (set `local.ClosestHit` _array_element)
        (set `self.ClosestImpactPoint` _screenposition)))
    ;[1 1 1 0.33] Adjust Circles only when new target
    (if (!= _hitcomponent (`self.CurrentTarget`))
      (set `self.CurrentTarget` _hitcomponent)
      (`self.AdjustCircles` (`KismetSystemLibrary.GetComponentBounds` _hitcomponent)))
    ;[1 1 1 0.33] Return Closest Hit To Screen Location
    (return true (`local.HitToScreen`))
    (else
      (return false (`self.ScreenCenter`)))))

(fn `GetSphereTracePoints`
  (returns (Start :type "Vector Structure") (End :type "Vector Structure"))
  (bind (_worldposition _worlddirection) (`GameplayStatics.DeprojectScreenToWorld` (`self.PlayerController`) (`self.ScreenCenter`)))
  (return (+ _worldposition (* _worlddirection (`self.SphereTraceStartOffset`))) (+ _worldposition (* _worlddirection (`self.SphereTraceRange`)))))

(fn `InitializeAimAssist`
  (params (PlayerController :type "PlayerController Object Reference"))
  (bind _playercontroller (`self.PlayerController`))
  (set `self.PlayerController` PlayerController)
  (if (`self.bIsDebugActivated`)
    (`PlayerController.ClientSetHUD` _playercontroller "/Game/External/AimAssit/Debug/HUD_AimAssist.HUD_AimAssist_C")
    (bind _output_get (set `self.AimAssistHUD` (cast `/Game/External/AimAssit/Debug/HUD_AimAssist` (`PlayerController.GetHUD` _playercontroller) :!pure true)))
    (`/Game/External/AimAssit/Debug/HUD_AimAssist.InitializeCircles` _output_get (`|MakeArray` (`self.BendZoneRadius`) (`self.SnapZoneRadius`) (`self.MagneticZoneRadius`)))
    (else
      (`self.AimAssistHUD`
        (:`then`
          (set `self.AimAssistHUD` null)
          (`self.ResetHUD`))
        (:`else`)))))

(fn `ResetCamera`
  (set `self.AdjustCrossHairLocatin` (`self.ScreenCenter`))
  (set `self.AimAssistMultiplier` 1.0)
  (set `self.Assist State` "")
  (set `self.Color Current State` (struct :`A` 1.0))
  (set `self.bShouldAdjustImpact` false))

(fn `ResetHUD`
  (`PlayerController.ClientSetHUD` (`self.PlayerController`) "/Script/Engine.HUD"))

(fn `StartAimAssist`
  (set `self.bIsPlayerAiming` true))

(fn `StopAimAssist`
  (set `self.bIsPlayerAiming` false)
  (set `self.AimAssistMultiplier` 1.0))

(fn `UpdateHUD`
  (bind _aimassisthud (`self.AimAssistHUD`))
  (if (`self.bIsDebugActivated`)
    (set `/Game/External/AimAssit/Debug/HUD_AimAssist.CrossHairLocation` (`self.AdjustCrossHairLocatin`) _aimassisthud)
    (set `/Game/External/AimAssit/Debug/HUD_AimAssist.ColorCurrentState` (`self.Color Current State`) _aimassisthud)
    (set `/Game/External/AimAssit/Debug/HUD_AimAssist.AssistState` (`self.Assist State`) _aimassisthud)))

(fn `UpdateInputDirection`
  (params (InInputDirection :type "Vector2D Structure"))
  ;[1 1 1 0.33] Check if Velocity is Near Zero
  (if (not (`KismetMathLibrary.IsNearlyZero2D` InInputDirection))
    ;[1 1 1 0.25] Update Rotation velocity
    (set `self.Input Direction` InInputDirection)
    (set `self.RotationVelocity` (`KismetMathLibrary.VSize2D` InInputDirection))
    ;[1 1 1 0.33] Check if velocity too low
    (if (not (<= (`self.RotationVelocity`) 0.1))
      ;[1 1 1 0.25] Enable Aim Assist when Player is trying to aim properly
      (set `self.bIsAssistEnable` true)
      ;;[1 0 0.05072 0.33] Reset Low Velocity Timer
      (set `self.bTriggerLowVelocity` false)
      (set `self.LowVelocityTimer` 0.0))
    (else
      ;[1 1 1 0.33] Trigger Low velocity to lock a target
      (set `self.bTriggerLowVelocity` true))))

(fn `UpdateLockState`
  (params (DeltaSec :type "Float (single-precision)"))
  (`/Game/o_Libraries/BPL_GeneralUtilities.Increase Value Float` (`self.LowVelocityTimer`) DeltaSec)
  (if (not (<= (`self.LowVelocityTimer`) (`self.LockStateDuration`)))
    (`self.ResetCamera`)
    (set `self.bIsAssistEnable` false)
    (set `self.bTriggerLowVelocity` false)
    (`self.UpdateHUD`)))