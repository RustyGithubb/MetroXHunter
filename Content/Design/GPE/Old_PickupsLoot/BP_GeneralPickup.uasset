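; BP_GeneralPickup is an interactable loot pickup that adds an amount of a pickup type, such as ammo or syringe liquid, to the player inventory.
; On BeginPlay it caches its interactable widget and sets the icon matching the pickup type.
; On interact it keeps whatever amount the inventory returns.
; At zero, if the player's interaction component is valid, it unregisters from nearby interactables and destroys itself.
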(event `self.ReceiveBeginPlay`
  (bind _aswbp_interactable (cast `/Game/Design/Widgets/WBP_Interactable` (`WidgetComponent.GetWidget` (`self.Widget`))))
  (set `self.InteractableWidget` _aswbp_interactable)
  (`self.EditSprite`))

(event `self.InteractableComponent.OnInteract`
  (bind _interactablecomponent (`self.InteractableComponent`))
  ;[1 1 1 0.33] INTERACT
  (bind _returnvalue (`InventoryComponent.AddToInventory` (`self.PlayerInventory`) (`self.PickupType`) (`self.Amount`)))
  (bind _output_get (set `self.Amount` _returnvalue))
  (if (== _output_get 0)
    (bind _playerinteractioncomponent (`/Game/Design/GPE/Old_Interactables/BP_InteractableComponent.PlayerInteractionComponent` _interactablecomponent)
      (:`then`
        (`/Game/Design/GPE/Old_Interactables/BP_InteractionComponent.RemoveNearInteractable` _playerinteractioncomponent _interactablecomponent)
        (`self.K2_DestroyActor`))
      (:`else`))))

(fn `EditSprite`
  (bind _sprite (`/Game/Design/Widgets/WBP_Interactable.Sprite` (`self.InteractableWidget`)))
  (switch `EPickupType` (`self.PickupType`)
    (:`Ammo`
      (`Image.SetBrush` _sprite (make `SlateBrush` "Image" "NoTile" "NoMirror" (make `DeprecateSlateVector2D` 50.0 50.0) (struct) (struct :`SpecifiedColor` (struct :`R` 1.0 :`G` 1.0 :`B` 1.0 :`A` 1.0) :`ColorUseRule` "UseColor_Specified") (struct :`CornerRadii` (struct) :`Color` (struct :`SpecifiedColor` (struct) :`ColorUseRule` "UseColor_Specified") :`RoundingType` "HalfHeightRadius") "/Game/Art/UI/Sprites/Placeholder/ammo_Sprite.ammo_Sprite")))
    (:`Syringe`
      (`Image.SetBrush` _sprite (make `SlateBrush` "Image" "NoTile" "NoMirror" (make `DeprecateSlateVector2D` 50.0 50.0) (struct) (struct :`SpecifiedColor` (struct :`R` 1.0 :`G` 1.0 :`B` 1.0 :`A` 1.0) :`ColorUseRule` "UseColor_Specified") (struct :`CornerRadii` (struct) :`Color` (struct :`SpecifiedColor` (struct) :`ColorUseRule` "UseColor_Specified") :`RoundingType` "HalfHeightRadius") "/Game/Art/UI/Sprites/Placeholder/Doctor-Needle-PNG-Clipart_Sprite.Doctor-Needle-PNG-Clipart_Sprite")))))

(fn `NewFunction`
  (returns (NewParam :type Boolean) (NewParam1 :type Boolean) (NewParam2 :type Boolean))
  (return false false false))

(fn `UserConstructionScript`)