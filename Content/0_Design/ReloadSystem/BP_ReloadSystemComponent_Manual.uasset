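; Manual reload component where the player loads Normal, Incendiary or Poison bullets one at a time, or unloads the whole magazine.
; Reload input toggles an active state that gates those inputs, locks gun fire and shows an input helper, with optional rules for full magazines and input release.
; The magazine is a stack of ammo types, pre-filled with Normal, popped on each shot and mirrored to a HUD widget.
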(event `self.ReceiveBeginPlay`
  (`self.CreateWidget`)
  ;[1 1 1 0.33] Initialize magazine
  (set `/Game/0_Design/GameManagement_/BP_Gun.IndexMagazineAmmo` 0 (`self.Gun`))
  (`self.FillMagazine` "NewEnumerator0")
  (add `/Game/0_Design/GameManagement_/BP_Gun.OnFire` (`self.Gun`) (delegate `OnGunFire`)))

(event `self.ReceiveEndPlay`
  (params (EndPlayReason :type "EEndPlayReason Enum" :default "Destroyed"))
  (bind _widget (`self.Widget`)
    (:`then`
      (`Widget.RemoveFromParent` _widget))
    (:`else`)))

(event `OnGunFire`
  (bind _magazine (`self.Magazine`))
  (`KismetArrayLibrary.Array_Remove` _magazine (- (`KismetArrayLibrary.Array_Length` _magazine) 1))
  (`self.UpdateMagazineWidget`))

(event `EnhancedInput|/Game/0_Design/GameManagement_/Input/IA_Reload_Manual1`
  (params (ActionValue :type Boolean) (ElapsedSeconds :type "Float (double-precision)") (TriggeredSeconds :type "Float (double-precision)") (InputAction :type "InputAction Object Reference" :default "/Game/0_Design/GameManagement_/Input/IA_Reload_Manual1.IA_Reload_Manual1"))
  (:`Started`
    ;[1 1 1 0.33] TODO: replace w/ custom Mapping Context
    (if (and (`self.IsReloadActive`) (not (`/Game/0_Design/GameManagement_/BP_Gun.IsGunFull` (`self.Gun`))))
      (`self.AddBulletInMagazine` "NewEnumerator0")
      (`KismetSystemLibrary.PrintText` "ReloadSystem: add 'Normal' bullet")
      (if (and (`self.ShouldDisableOnFill`) (`/Game/0_Design/GameManagement_/BP_Gun.IsGunFull` (`self.Gun`))) :!label _label
        (`self.SetReloadActive` false)
        (`KismetSystemLibrary.PrintText` "ReloadSystem: disabling reload, magazine is full!")))))

(event `EnhancedInput|/Game/0_Design/GameManagement_/Input/IA_Reload_Manual2`
  (params (ActionValue :type Boolean) (ElapsedSeconds :type "Float (double-precision)") (TriggeredSeconds :type "Float (double-precision)") (InputAction :type "InputAction Object Reference" :default "/Game/0_Design/GameManagement_/Input/IA_Reload_Manual2.IA_Reload_Manual2"))
  (:`Started`
    ;[1 1 1 0.33] TODO: replace w/ custom Mapping Context
    (if (and (`self.IsReloadActive`) (not (`/Game/0_Design/GameManagement_/BP_Gun.IsGunFull` (`self.Gun`))))
      (`self.AddBulletInMagazine` "NewEnumerator1")
      (`KismetSystemLibrary.PrintText` "ReloadSystem: add 'Incendiary' bullet")
      (goto _label))))

(event `EnhancedInput|/Game/0_Design/GameManagement_/Input/IA_Reload_Manual3`
  (params (ActionValue :type Boolean) (ElapsedSeconds :type "Float (double-precision)") (TriggeredSeconds :type "Float (double-precision)") (InputAction :type "InputAction Object Reference" :default "/Game/0_Design/GameManagement_/Input/IA_Reload_Manual3.IA_Reload_Manual3"))
  (:`Started`
    ;[1 1 1 0.33] TODO: replace w/ custom Mapping Context
    (if (and (`self.IsReloadActive`) (not (`/Game/0_Design/GameManagement_/BP_Gun.IsGunFull` (`self.Gun`))))
      (`self.AddBulletInMagazine` "NewEnumerator2")
      (`KismetSystemLibrary.PrintText` "ReloadSystem: add 'Poison' bullet")
      (goto _label))))

(event `EnhancedInput|/Game/0_Design/GameManagement_/Input/IA_Reload_ManualUnload`
  (params (ActionValue :type Boolean) (ElapsedSeconds :type "Float (double-precision)") (TriggeredSeconds :type "Float (double-precision)") (InputAction :type "InputAction Object Reference" :default "/Game/0_Design/GameManagement_/Input/IA_Reload_ManualUnload.IA_Reload_ManualUnload"))
  (:`Started`
    ;[1 1 1 0.33] TODO: replace w/ custom Mapping Context
    (if (and (`self.IsReloadActive`) (not (`/Game/0_Design/GameManagement_/BP_Gun.IsGunEmpty` (`self.Gun`))))
      (`self.UnloadMagazine`)
      (`KismetSystemLibrary.PrintText` "ReloadSystem: unload magazine!"))))

(fn `AddBulletInMagazine`
  (params (`Ammo Type` :type "/Game/0_Design/ReloadSystem/Enums/E_ManualAmmoType Enum" :default "NewEnumerator0"))
  (`/Engine/EditorBlueprintResources/StandardMacros.IncrementInt` (`/Game/0_Design/GameManagement_/BP_Gun.IndexMagazineAmmo` (`self.Gun`))
    (:`  `
      (`KismetArrayLibrary.Array_Add` (`self.Magazine`) `Ammo Type`)
      (`self.UpdateMagazineWidget`))))

(fn `CreateWidget`
  (bind _asbpc_controller (cast `/Game/0_Design/GameManagement_/BPC_Controller` (`Pawn.GetController` (`self.PlayerCharacter`))))
  (bind _returnvalue (`|CreateWidget` "/Game/UI/Widgets/WBP_ReloadSystem_Manual.WBP_ReloadSystem_Manual_C" _asbpc_controller))
  (bind _output_get (set `self.Widget` _returnvalue))
  (`UserWidget.AddToViewport` _output_get 0))

(fn `FillMagazine`
  (params (`Ammo Type` :type "/Game/0_Design/ReloadSystem/Enums/E_ManualAmmoType Enum" :default "NewEnumerator0"))
  (bind _gun (`self.Gun`))
  (bind _gun_2 (`self.Gun`))
  (for _ (range (`/Game/0_Design/GameManagement_/BP_Gun.IndexMagazineAmmo` _gun) (`/Game/0_Design/GameManagement_/BP_Gun.MaxMagazineAmmo` _gun))
    (`KismetArrayLibrary.Array_Add` (`self.Magazine`) `Ammo Type`))
  (set `/Game/0_Design/GameManagement_/BP_Gun.IndexMagazineAmmo` (`/Game/0_Design/GameManagement_/BP_Gun.MaxMagazineAmmo` _gun_2) _gun_2)
  (`self.UpdateMagazineWidget`))

(fn `IsLockingGunFire`
  (returns (IsFireLocked :type Boolean))
  (return (`self.IsReloadActive`)))

(fn `OnReloadInput`
  (params (`Input Type` :type "/Game/0_Design/E_InputActionType Enum" :default "NewEnumerator0"))
  (if (`self.ShouldPreventReloadOnFull`)
    ;[1 1 1 0.33] Prevent reloading on full
    (if (not (`/Game/0_Design/GameManagement_/BP_Gun.IsGunFull` (`self.Gun`)))
      (switch `/Game/0_Design/E_InputActionType` `Input Type` :!label _label
        (:`NewEnumerator1`
          (`self.SetReloadActive` true)
          (`KismetSystemLibrary.PrintText` "ReloadSystem: activating reload, input started!"))
        (:`NewEnumerator3`
          (if (`self.ShouldDisableOnRelease`)
            (`self.SetReloadActive` false)
            (`KismetSystemLibrary.PrintText` "ReloadSystem: disabling reload, input released!"))))
      (else
        (`KismetSystemLibrary.PrintText` "ReloadSystem: can't reload, magazine is full!" true true (struct :`R` 1.0 :`A` 1.0) 2.0 "ReloadSystemUnableMagazineFull")))
    (else
      (goto _label))))

(fn `SetReloadActive`
  (params (IsActive :type Boolean))
  (bind _output_get (set `self.IsReloadActive` IsActive))
  (`/Game/UI/Widgets/WBP_ReloadSystem_Manual.ShowInputHelper` (`self.Widget`) _output_get))

(fn `UnloadMagazine`
  (set `/Game/0_Design/GameManagement_/BP_Gun.IndexMagazineAmmo` 0 (`self.Gun`))
  (`KismetArrayLibrary.Array_Clear` (`self.Magazine`))
  (`self.UpdateMagazineWidget`))

(fn `UpdateMagazineWidget`
  (`/Game/UI/Widgets/WBP_ReloadSystem_Manual.UpdateMagazine` (`self.Widget`) self))