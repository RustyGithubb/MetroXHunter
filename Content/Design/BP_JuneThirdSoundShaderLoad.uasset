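; An actor that appears to warm up effects and sounds, so their shaders and audio load before gameplay needs them.
; On BeginPlay it spawns several Niagara systems at its own location, including muzzle flash, lightning and dust, plus an actor of unspecified class.
; It also plays the gunshot and creature sound cues there at near-zero volume, making them effectively inaudible.
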(event `self.ReceiveBeginPlay`
  (bind _returnvalue_location (`KismetMathLibrary.BreakTransform` (`self.GetTransform`)))
  (bind _returnvalue_location_2 (`KismetMathLibrary.BreakTransform` (`self.GetTransform`)))
  (`NiagaraFunctionLibrary.SpawnSystemAtLocation` "/Game/Art/VFX/NS_Gun/NS_Shoot_Distortion.NS_Shoot_Distortion" _returnvalue_location)
  (`NiagaraFunctionLibrary.SpawnSystemAtLocation` "/Game/Art/VFX/NS_Gun/NS_Muzzle_Flash_Multiple.NS_Muzzle_Flash_Multiple" _returnvalue_location)
  (`NiagaraFunctionLibrary.SpawnSystemAtLocation` "/Game/Art/VFX/NS_Electrics/NS_Generator_Lightning.NS_Generator_Lightning" _returnvalue_location)
  (`NiagaraFunctionLibrary.SpawnSystemAtLocation` "/Game/Art/VFX/NS_FogDust/NS_Dust.NS_Dust" _returnvalue_location)
  (`NiagaraFunctionLibrary.SpawnSystemAtLocation` "/Game/Art/VFX/NS_FogDust/NS_Dust_Falling_Grain.NS_Dust_Falling_Grain" _returnvalue_location)
  (`|SpawnActorFromClass` null (`self.GetTransform`) "Undefined" "MultiplyWithRoot" null null)
  (`GameplayStatics.PlaySoundAtLocation` "/Game/Sounds/Placeholders/Character/Gun/SC_GunShot.SC_GunShot" _returnvalue_location_2 (struct) 1e-05 1.0 0.0 null null null null)
  (`GameplayStatics.PlaySoundAtLocation` "/Game/Sounds/Placeholders/Spiders/Attack/SC_SpiderAttack.SC_SpiderAttack" _returnvalue_location_2 (struct) 1e-05 1.0 0.0 null null null null)
  (`GameplayStatics.PlaySoundAtLocation` "/Game/Sounds/Placeholders/SculkShriekers/SC_CreatureShriek.SC_CreatureShriek" _returnvalue_location_2 (struct) 1e-05 1.0 0.0 null null null null)
  (`GameplayStatics.PlaySoundAtLocation` "/Game/Sounds/Placeholders/Spiders/Movement/SC_SpiderMovement.SC_SpiderMovement" _returnvalue_location_2 (struct) 1e-05 1.0 0.0 null null null null))

(fn `UserConstructionScript`)