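; Cinematic variant of a double 4x4 door that plays a sequence when opened through its SetDoorOpened event.
; With a valid interactable, it freezes and removes the interaction, saves it as consumed, then triggers the SequencerCinematic component.
; When the sequence ends, or immediately if no interactable is valid, both leaves snap to mirrored final yaw rotations.
; It has no closing logic.
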(event `self.SetDoorOpened`
  (params (bShouldOpen :type Boolean))
  (if bShouldOpen
    (set `self.bIsOpened` true)
    (`self.InteractableComponent`
      (:`then`
        (`self.SetInteractionFreezed` true)
        (`self.RemoveInteractionComponent`)
        (`self.SaveConsumeInteraction` true)
        (`/Game/Design/EnvironmentEvents/Components/BP_TriggerEventReceiver_Component.OnPlayComponentSpecificEvent` (`self.SequencerCinematic`) true null))
      (:`else`
        (`SceneComponent.K2_SetRelativeRotation` (`self.L_Door`) (`KismetMathLibrary.MakeRotator` 0.0 0.0 (+ (* 1.0 (`self.FinalRotation`)) (`self.LStartYawRotation`))) false false :!label _label)
        (`SceneComponent.K2_SetRelativeRotation` (`self.R_Door`) (`KismetMathLibrary.MakeRotator` 0.0 0.0 (+ (* 1.0 (* (`self.FinalRotation`) -1.0)) (`self.RStartYawRotation`))) false false)))))

(event `self.SequencerCinematic.OnSequenceEnd`
  (goto _label))

(fn `UserConstructionScript`
  (`parent.UserConstructionScript`))