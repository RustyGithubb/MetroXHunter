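; Level-design trigger box that fires environment events on overlap, gated by optional player flag values.
; It gathers receiver components from itself and a linked actor, calls their enter and exit hooks, and runs a linked ScriptedEventManager on enter.
; One-time boxes destroy their components on exit and save that state, replaying loadable receivers on load.
; The construction script sizes a labelled, color-coded visualizer cube.
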(event `self.ReceiveBeginPlay`
  (`KismetSystemLibrary.DelayUntilNextTick`)
  (`|ExecutionSequence`
    (:`then_1`
      (if (`self.bShouldSpawn`)
        (`|ExecutionSequence`
          (:`then_0`
            ;[1 1 1 0.33] Should Show Ingame? (for debug purposes probably)
            (`SceneComponent.SetHiddenInGame` (`self.DONT_MOVE_TriggerBox`) (not (`self.ShowIngame`)) false)
            (`SceneComponent.SetHiddenInGame` (`self.TextRender`) (not (`self.ShowIngame`)) false)
            (`SceneComponent.SetHiddenInGame` (`self.VisualizerCube`) (not (`self.ShowIngame`)) false)
            ;[1 1 1 0.33] Cache Player FlagComponent if we need to check flags
            (if (`BlueprintMapLibrary.Map_IsNotEmpty` (`self.NecessaryFlags`))
              (set `self.CharacterFlagComponent` (`self.GetComponentByClass` (`GameplayStatics.GetPlayerPawn` 0) "/Game/Design/EnvironmentEvents/BP_EventFlagsComponent.BP_EventFlagsComponent_C"))))
          (:`then_1`
            (`self.GetReceiverComponent Metro Actualise`)))))))

(event `self.DONT_MOVE_TriggerBox.OnComponentBeginOverlap`
  (params (OverlappedComponent :type "PrimitiveComponent Object Reference") (OtherActor :type "Actor Object Reference") (OtherComp :type "PrimitiveComponent Object Reference") (OtherBodyIndex :type Integer) (bFromSweep :type Boolean) (SweepResult :type "HitResult Structure (by ref)"))
  (bind _everythingright (`self.AreFlagsCorrect`))
  (if _everythingright
    (for _array_element (`self.ComponentsToCall`)
      (`/Game/Design/EnvironmentEvents/Components/BP_TriggerEventReceiver_Component.OnTriggerBoxEnter` _array_element self))
    (bind _asscripted_event_manager (cast `ScriptedEventManager` (`self.LinkedReceiverActor`)))
    (`ScriptedEventManager.RunScriptedEvents` _asscripted_event_manager)))

(event `self.DONT_MOVE_TriggerBox.OnComponentEndOverlap`
  (params (OverlappedComponent :type "PrimitiveComponent Object Reference") (OtherActor :type "Actor Object Reference") (OtherComp :type "PrimitiveComponent Object Reference") (OtherBodyIndex :type Integer))
  (bind _everythingright (`self.AreFlagsCorrect`))
  (if _everythingright
    (for _array_element (`self.ComponentsToCall`)
      (`/Game/Design/EnvironmentEvents/Components/BP_TriggerEventReceiver_Component.OnTriggerBoxExit` _array_element self))
    ;[1 0.4063 0.3165 0.33] Should Destroy after One-Time Use?
    (if (`self.OneTimeUse`)
      (`self.RemoveComponents`))))

(event `self.SaveLoad.OnLoadActor`
  (bind _value (`StructUtilsFunctionLibrary.GetInstancedStructValue` (`SaveLoadComponent.SavedData` (`self.SaveLoad`)))
    (:`Valid`
      (bind _output_get (set `self.bShouldSpawn` (`.bShouldSpawn` (break `BaseSavedData` _value))))
      (if (not _output_get)
        (`self.GetReceiverComponent Metro Actualise`)
        (for _array_element (`self.ComponentsToCall`)
          (if (`/Game/Design/EnvironmentEvents/Components/BP_TriggerEventReceiver_Component.bShouldLoad` _array_element)
            (`/Game/Design/EnvironmentEvents/Components/BP_TriggerEventReceiver_Component.OnLoad` _array_element)
            (set `self.MaxDelayBeforeActivation` (`KismetMathLibrary.FMax` (`/Game/Design/EnvironmentEvents/Components/BP_TriggerEventReceiver_Component.DelayBeforeActivation` _array_element) (`self.MaxDelayBeforeActivation`)))))
        (`KismetSystemLibrary.Delay` (`self.MaxDelayBeforeActivation`))
        (`self.RemoveComponents`)))))

(fn `AreFlagsCorrect`
  (returns (EverythingRight :type Boolean))
  (locals (Keys :type "Array of GameplayTag Structure") (Values :type "Array of Boolean") (isRight :type Boolean))
  (`self.CharacterFlagComponent`
    (:`then`
      (`|ExecutionSequence`
        (:`then_0`
          ;[1 1 1 0.33] Caching
          (bind _keys (`BlueprintMapLibrary.Map_Keys` (`self.NecessaryFlags`)))
          (set `local.Keys` _keys)
          (bind _values (`BlueprintMapLibrary.Map_Values` (`self.NecessaryFlags`)))
          (set `local.Values` _values)
          (set `local.isRight` true))
        (:`then_1`
          (for (_array_element _array_index) (`local.Keys`)
            (if (not (== (`/Game/Design/EnvironmentEvents/BP_EventFlagsComponent.GetFlagValue` (`self.CharacterFlagComponent`) _array_element) (`|GetArrayItem` (`local.Values`) _array_index)))
              (set `local.isRight` false)
              (break)))
          (return (`local.isRight`)))))
    (:`else`
      ;[1 1 1 0.33] No flags to check?
      ; Good to go!
      (return true))))

(fn `GetReceiverComponent`
  ;[0.04963 0.5881 1 0.33] Is this Box connected to an external Actor that stores the Components?
  (bind _linkedreceiveractor (`self.LinkedReceiverActor`)
    (:`then`
      ;[1 0.9531 0.4163 0.33] Does this linked Actor have Components?
      (`/Engine/EditorBlueprintResources/StandardMacros.IsValid` (`self.GetComponentByClass` _linkedreceiveractor "/Game/Design/EnvironmentEvents/Components/BP_TriggerEventReceiver_Component.BP_TriggerEventReceiver_Component_C")
        (:`Is Valid`
          ;[1 0.4331 0.6261 0.33] If yes save all Components
          (set `self.ComponentsToCall` (`self.K2_GetComponentsByClass` (`self.LinkedReceiverActor`) "/Game/Design/EnvironmentEvents/Components/BP_TriggerEventReceiver_Component.BP_TriggerEventReceiver_Component_C")))
        (:`Is Not Valid`
          (cast `ScriptedEventManager` _linkedreceiveractor
            (:`CastFailed`
              ;[0.4676 1 0.4728 0.33] Else Print Error
              (if (not (`self.DontPrintError`)) :!label _label
                (`KismetSystemLibrary.PrintText` (`|FormatText` "TriggerBoxEvent with name {name} doesn't possess any Trigger Receiver Component itself; and isn't linked to an Actor possessing one. \nTo prevent this error, check the \"Don't Print Error\" on the TriggerBox" (`KismetSystemLibrary.GetDisplayName` self)) true true (struct :`R` 1.0 :`A` 1.0) 5000.0)))))))
    (:`else`
      ;[0.5071 0.3153 1 0.33] Or are components stored on this Trigger?
      (bind _output_get (set `self.ComponentsToCall` (`self.K2_GetComponentsByClass` "/Game/Design/EnvironmentEvents/Components/BP_TriggerEventReceiver_Component.BP_TriggerEventReceiver_Component_C")))
      (if (not (`KismetArrayLibrary.Array_IsNotEmpty` _output_get))
        (goto _label)))))

(fn `GetReceiverComponent Metro Actualise`
  (`|ExecutionSequence`
    (:`then_0`
      ;[0.5071 0.3153 1 0.33] Or are components stored on this Trigger?
      (bind _output_get (set `self.ComponentsToCall` (`self.K2_GetComponentsByClass` "/Game/Design/EnvironmentEvents/Components/BP_TriggerEventReceiver_Component.BP_TriggerEventReceiver_Component_C")))
      (if (not (`KismetArrayLibrary.Array_IsNotEmpty` _output_get))
        ;[0.4676 1 0.4728 0.33] Else Print Error
        (if (not (`self.DontPrintError`)) :!label _label
          (`KismetSystemLibrary.PrintText` (`|FormatText` "TriggerBoxEvent with name {name} doesn't possess any Trigger Receiver Component itself; and isn't linked to an Actor possessing one. \nTo prevent this error, check the \"Don't Print Error\" on the TriggerBox" (`KismetSystemLibrary.GetDisplayName` self)) true true (struct :`R` 1.0 :`A` 1.0) 5000.0))))
    (:`then_1`
      ;[0.04963 0.5881 1 0.33] Is this Box connected to an external Actor that stores the Components?
      (bind _linkedreceiveractor (`self.LinkedReceiverActor`)
        (:`then`
          ;[1 0.9531 0.4163 0.33] Does this linked Actor have Components?
          (`/Engine/EditorBlueprintResources/StandardMacros.IsValid` (`self.GetComponentByClass` _linkedreceiveractor "/Game/Design/EnvironmentEvents/Components/BP_TriggerEventReceiver_Component.BP_TriggerEventReceiver_Component_C")
            (:`Is Valid`
              ;[1 0.4331 0.6261 0.33] If yes save all Components
              (for _array_element (`self.K2_GetComponentsByClass` (`self.LinkedReceiverActor`) "/Game/Design/EnvironmentEvents/Components/BP_TriggerEventReceiver_Component.BP_TriggerEventReceiver_Component_C")
                (`KismetArrayLibrary.Array_Add` (`self.ComponentsToCall`) _array_element)))
            (:`Is Not Valid`
              (cast `ScriptedEventManager` _linkedreceiveractor
                (:`CastFailed`
                  (goto _label))))))
        (:`else`)))))

(fn `RemoveComponents`
  (for _array_element (`|MakeArray` (`self.DONT_MOVE_TriggerBox`) (`self.TextRender`) (`self.VisualizerCube`) :!type "ActorComponent Object Reference")
    (`/Engine/EditorBlueprintResources/StandardMacros.IsValid` _array_element
      (:`Is Valid`
        (`ActorComponent.K2_DestroyComponent` _array_element))))
  (`self.SaveDeath`))

(fn `SaveDeath`
  (bind _saveload (`self.SaveLoad`))
  (bind _saveddata (`SaveLoadComponent.SavedData` _saveload))
  (bind _value (`StructUtilsFunctionLibrary.GetInstancedStructValue` _saveddata)
    (:`Valid`
      (bind _structout (setmembers `BaseSavedData` :`StructRef` _value :`bShouldSpawn` false))
      (`StructUtilsFunctionLibrary.SetInstancedStructValue` _saveddata _structout)
      (`SaveLoadComponent.Save` _saveload))))

(fn `UserConstructionScript`
  (bind (_boxsizehandle_x _boxsizehandle_y) (`KismetMathLibrary.BreakVector` (`self.BoxSizeHandle`)))
  (`self.TextMaterial`
    (:`then`
      _)
    (:`else`
      (bind _returnvalue (`PrimitiveComponent.CreateDynamicMaterialInstance` (`self.TextRender`) 0 "/Game/Art/0_Materials/Debug/M_CameraAlignedText.M_CameraAlignedText" "None"))
      (set `self.TextMaterial` _returnvalue)))
  ;[0 0 0 0.33] Set the correct size for the Trigger Box, the "OneTimeUse" visualizer box, and the Text inside (so it doesn't get too long)
  (`SceneComponent.K2_SetRelativeLocation` (`self.DONT_MOVE_TriggerBox`) (0.0 0.0 0.0) false false)
  (`BoxComponent.SetBoxExtent` (`self.DONT_MOVE_TriggerBox`) (`self.BoxSizeHandle`) false)
  (`SceneComponent.SetRelativeScale3D` (`self.VisualizerCube`) (* (`self.BoxSizeHandle`) 0.02))
  (`TextRenderComponent.SetWorldSize` (`self.TextRender`) (* (`KismetMathLibrary.FMax` (`KismetMathLibrary.Abs` _boxsizehandle_x) (`KismetMathLibrary.Abs` _boxsizehandle_y)) 0.2 (`self.TextScaleMultiplier`)))
  ;[0 0 0 0.33] Red if the TriggerBox is one-time-use
  ; Blue otherwise
  (`PrimitiveComponent.SetMaterial` (`self.VisualizerCube`) 0 (select `bool` (`self.OneTimeUse`) :`false` "/Game/Art/0_Materials/Debug/Instances/MI_TranslucentBlue.MI_TranslucentBlue" :`true` "/Game/Art/0_Materials/Debug/Instances/MI_TranslucentRed.MI_TranslucentRed" :!type "MaterialInterface Object Reference"))
  ;[0 0 0 0.33] Set a custom visible name.
  ; I could use the "FitTextToNumberOfCharacters" but with the camera-oriented text and many different sizes possible for the TriggerBox, the LD is better of making line breaks themselves...
  (`TextRenderComponent.K2_SetText` (`self.TextRender`) (`self.TriggerCustomName`))
  ;[0 0 0 0.33] TextColor & Emissive
  (`TextRenderComponent.SetTextRenderColor` (`self.TextRender`) (`KismetMathLibrary.Conv_LinearColorToColor` (`self.TextColor`)))
  (`MaterialInstanceDynamic.SetScalarParameterValue` (`self.TextMaterial`) "TextEmissive" (`self.TextEmissiveIntensity`))
  ;[1 1 1 0.33] HIDDEN QUAND EDITOR
  (`SceneComponent.SetHiddenInGame` (`self.DONT_MOVE_TriggerBox`) (not (`self.ShowIngame`)) false)
  (`SceneComponent.SetHiddenInGame` (`self.TextRender`) (not (`self.ShowIngame`)) false)
  (`SceneComponent.SetHiddenInGame` (`self.VisualizerCube`) (not (`self.ShowIngame`)) false))