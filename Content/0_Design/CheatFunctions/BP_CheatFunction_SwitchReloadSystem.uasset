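; Cheat function that switches the player character's reload system to one chosen from a list of reload system classes.
; On init it sets the max value from the list length, waits a tick, caches the controlled BP_MainChara, and sets the current value to the index of its active reload system.
; When triggered, it creates the reload system at the selected index on the character and prints its name.
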(event `self.OnInit`
  ;[1 1 1 0.33] Auto-Fill Max Value
  (set `self.MaxValue` (`KismetMathLibrary.Conv_IntToDouble` (- (`KismetArrayLibrary.Array_Length` (`self.ReloadSystemClasses`)) 1)))
  (`KismetSystemLibrary.DelayUntilNextTick`)
  (`self.Get References`)
  ;[1 1 1 0.33] Auto-Fill the Current ReloadSystem as value
  (for (_array_element _array_index) (`self.ReloadSystemClasses`)
    (if (== _array_element (`GameplayStatics.GetObjectClass` (`/Game/0_Design/GameManagement_/BP_MainChara.CurrentReloadSystem` (`self.PlayerCharacter`))))
      (set `self.Value` (`KismetMathLibrary.Conv_IntToDouble` _array_index))
      (break))))

(event `self.OnCheat`
  (bind _output (`|GetArrayItem` (`self.ReloadSystemClasses`) (`KismetMathLibrary.FTrunc` (`self.Value`))))
  (`/Game/0_Design/GameManagement_/BP_MainChara.CreateReloadSystem` (`self.PlayerCharacter`) _output)
  (`KismetSystemLibrary.PrintText` (`|FormatText` "Cheat: Switching to Reload System '{Name}'" (`KismetSystemLibrary.GetClassDisplayName` _output)) true true (struct :`G` 0.66 :`B` 1.0 :`A` 1.0) 2.0 "CheatFunctionSwitchReloadSystem"))

(fn `Get References`
  (bind _asbp_main_chara (cast `/Game/0_Design/GameManagement_/BP_MainChara` (`Controller.K2_GetPawn` (`CheatManager.GetPlayerController` (`self.CheatManager`)))))
  (set `self.PlayerCharacter` _asbp_main_chara))