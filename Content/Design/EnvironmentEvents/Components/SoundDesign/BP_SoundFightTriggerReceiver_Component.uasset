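; Trigger receiver component that plays 2D fight music and drives it from the number of enemies attacking the player.
; When triggered, it spawns the sound and binds to the player's AITargetComponent attacker updates.
; With attackers present, a flag-guarded one-shot sends the start-fight parameter.
; At zero attackers, after a delay, it sends the stop parameter and unbinds, or fades out or stops if none is set.
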(event `StopMusic`
  (`KismetSystemLibrary.Delay` (`self.StopDelay`))
  (bind _audiocomponent (`self.AudioComponent`)
    (:`then`
      (if (!= (`self.StopFightParameter`) "None")
        (`AudioParameterControllerInterface.SetTriggerParameter` _audiocomponent (`self.StopFightParameter`))
        (remove `AITargetComponent.OnAttackersUpdate` (`self.AITargetComponent`) (`|CreateDelegate` :!event `OnUpdateMusicState`))
        (elif (> (`self.FadeOutTime`) 0.0)
          (`AudioComponent.FadeOut` _audiocomponent (`self.FadeOutTime`) 0.0 "Linear")
          (else
            (`AudioComponent.Stop` _audiocomponent)))))
    (:`else`)))

(fn `OnPlayComponentSpecificEvent`
  (params (FromBoxEnter :type Boolean) (TriggerBox :type "Actor Object Reference"))
  (set `self.AITargetComponent` (`Actor.GetComponentByClass` (`GameplayStatics.GetPlayerCharacter` 0) "/Script/MetroXHunter.AITargetComponent"))
  (bind _returnvalue (`GameplayStatics.SpawnSound2D` (`self.SoundAsset`) 1.0 1.0 0.0 null))
  (set `self.AudioComponent` _returnvalue)
  (add `AITargetComponent.OnAttackersUpdate` (`self.AITargetComponent`) (`|CreateDelegate` :!event `OnUpdateMusicState`)))

(fn `OnUpdateMusicState`
  (params (AITargetComponent :type "AITargetComponent Object Reference"))
  (if (== (`AITargetComponent.GetAttackersCount` AITargetComponent) 0)
    (`self.StopMusic`)
    (elif (`self.bIsInFight`)
      (`AudioParameterControllerInterface.SetTriggerParameter` (`self.AudioComponent`) (`self.StartFightParameter`))
      (set `self.bIsInFight` false))))