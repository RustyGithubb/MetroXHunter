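; Reload component that runs a Gears-style active reload quick-time event for the owner's gun.
; A looping timer advances a gauge; a second input grades the reload perfect, active or failed by timing, while no input gives a normal reload.
; Each outcome fills the magazine from inventory or infinite ammo, most after a computed delay, and fires tagged gameplay events.
; It updates gun and HUD through message calls, finding the gun among child actors.
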(event `InitializeReloadComponent`
  ;[1 0 0 0.33] BEGIN PLAY
  (`self.GetReferences` :!label _label)
  (`self.UpdateAmmoCount` (`self.MaxMagazineAmmoCount`)))

(event `self.ReceiveBeginPlay`
  (goto _label))

(event `StartReloadSequence`
  (if (not (`self.IsGunFireLocked`))
    (set `self.IsReloadActive` true)
    (set `self.CurrentGunState` "NewEnumerator2")
    ;[1 0 0 0.33 55] DATA DEBUG
    (`/EventDispatcherHub/FunctionLibrary/BPL_EventDispatcherHub.Call Single Gameplay Event` (struct :`TagName` "Event.ReloadSystem.StartReload") self)
    (`self.UpdateCurrentReloadState` "NewEnumerator0")
    (set `self.ReloadElapsedTime` 0.0)
    (bind _returnvalue (`KismetSystemLibrary.K2_SetTimerDelegate` (delegate `UpdateReloadGauge`) (`self.ReloadRefreshRate`) true))
    (set `self.TimerHandleReloadPlayback` _returnvalue)))

(event `UpdateReloadGauge`
  (set `self.ReloadElapsedTime` (+ (`self.ReloadElapsedTime`) (`self.ReloadRefreshRate`)))
  (`self.OnUpdateCursorPosition`)
  ;[0 1 0.9093] Normal Reload if the player don't trigger the button
  (if (>= (`self.ReloadElapsedTime`) (`self.NormalReloadDuration`))
    (`KismetSystemLibrary.K2_ClearAndInvalidateTimerHandle` (`self.TimerHandleReloadPlayback`))
    (`self.TriggerNormalReload`)))

(event `TriggerNormalReload`
  ;[0 1 0.9093] Normal Reload (Happen if the player do nothing, end of the gauge)
  (if (`self.UseInfiniteAmmo`)
    (`self.FinalizeReload` (`self.MaxMagazineAmmoCount`))
    (else
      (bind (_newmagazineammocount _inventoryammoconsumed) (`self.ComputeReloadAmmoAmount`))
      (`self.FinalizeReload` _newmagazineammocount "NewEnumerator0" 0.0 _inventoryammoconsumed)))
  (`self.UpdateCurrentReloadState` "NewEnumerator1")
  (`KismetSystemLibrary.Delay` (`self.NormalReloadAnimTime`))
  (set `self.IsReloadActive` false)
  (`/EventDispatcherHub/FunctionLibrary/BPL_EventDispatcherHub.Call Single Gameplay Event` (struct :`TagName` "Event.ReloadSystem.EndPassiveReload") self))

(event `TriggerActiveReload`
  ;[0 1 0.9093] Active Reload (Faster than Normal, Slower than Perfect, Grey part)
  (if (`self.UseInfiniteAmmo`)
    (`self.FinalizeReload` (`self.MaxMagazineAmmoCount`) "NewEnumerator3")
    (else
      (bind (_newmagazineammocount _inventoryammoconsumed) (`self.ComputeReloadAmmoAmount`))
      (`self.FinalizeReload` _newmagazineammocount "NewEnumerator3" (+ (- (`self.ActiveReloadEndTime`) (`self.ReloadElapsedTime`)) (`self.ActiveReloadAnimTime`)) _inventoryammoconsumed)))
  (`self.UpdateCurrentReloadState` "NewEnumerator4")
  (set `self.IsReloadActive` false)
  (`/EventDispatcherHub/FunctionLibrary/BPL_EventDispatcherHub.Call Single Gameplay Event` (struct :`TagName` "Event.ReloadSystem.EndActiveReload") self))

(event `TriggerPerfectReload`
  ;[0 1 0.9093] Perfect Reload (Fastest reload, white part)
  (if (`self.UseInfiniteAmmo`)
    (`self.FinalizeReload` (`self.MaxMagazineAmmoCount`) "NewEnumerator5")
    (else
      (bind (_newmagazineammocount _inventoryammoconsumed) (`self.ComputeReloadAmmoAmount`))
      (`self.FinalizeReload` _newmagazineammocount "NewEnumerator5" (+ (- (`self.ActiveReloadStartTime`) (`self.ReloadElapsedTime`)) (`self.PerfectReloadAnimTime`)) _inventoryammoconsumed)))
  (`self.UpdateCurrentReloadState` "NewEnumerator6")
  (set `self.IsReloadActive` false)
  (`/EventDispatcherHub/FunctionLibrary/BPL_EventDispatcherHub.Call Single Gameplay Event` (struct :`TagName` "Event.ReloadSystem.EndPerfectReload") self))

(event `TriggerFailedReload`
  ;[0 1 0.9093] Failed Reload (Slowest reload, dark parts)
  (if (`self.UseInfiniteAmmo`)
    (`self.FinalizeReload` (`self.MaxMagazineAmmoCount`) "NewEnumerator7")
    (else
      (bind (_newmagazineammocount _inventoryammoconsumed) (`self.ComputeReloadAmmoAmount`))
      (`self.FinalizeReload` _newmagazineammocount "NewEnumerator7" (+ (- (`self.NormalReloadDuration`) (`self.ReloadElapsedTime`)) (`self.FailedReloadPenaltyTime`)) _inventoryammoconsumed)))
  (`self.UpdateCurrentReloadState` "NewEnumerator8")
  (set `self.IsReloadActive` false) ; Lock the gun until the reload is finished
  (`/EventDispatcherHub/FunctionLibrary/BPL_EventDispatcherHub.Call Single Gameplay Event` (struct :`TagName` "Event.ReloadSystem.EndFailedReload") self))

(fn `ComputeReloadAmmoAmount`
  (returns (NewMagazineAmmoCount :type Integer) (InventoryAmmoConsumed :type Integer))
  (locals (AmmoToConsumeToMax :type Integer))
  ;[1 1 1 0.33] How much Ammo do we need to get to Max?
  (bind _currentammocount (message `/Game/0_Design/ReloadSystem/BPI_ReloadSystemGun.GetCurrentMagazineAmmoCount` (`self.CharacterGun`)))
  (set `local.AmmoToConsumeToMax` (- (`self.MaxMagazineAmmoCount`) _currentammocount))
  (if (>= (`/Game/0_Design/GameManagement_/BP_InventoryComponent.CurrentDefaultAmmoAmount` (`self.CharacterInventory`)) (`local.AmmoToConsumeToMax`))
    (return (`self.MaxMagazineAmmoCount`) (`local.AmmoToConsumeToMax`))
    (else
      (return (+ _currentammocount (`/Game/0_Design/GameManagement_/BP_InventoryComponent.CurrentDefaultAmmoAmount` (`self.CharacterInventory`))) (`/Game/0_Design/GameManagement_/BP_InventoryComponent.CurrentDefaultAmmoAmount` (`self.CharacterInventory`))))))

(fn `CreateWidget`)

(fn `GetAmmoData`
  (returns (IndexMagazinAmmo :type Integer) (MaxMagazinAmmo :type Integer))
  (bind _currentammocount (message `/Game/0_Design/ReloadSystem/BPI_ReloadSystemGun.GetCurrentMagazineAmmoCount` (`self.CharacterGun`)))
  (return _currentammocount (`self.MaxMagazineAmmoCount`)))

(fn `GetCurrentReloadState`
  (returns (CurrentReloadState :type "/Game/0_Design/ReloadSystem/Enums/E_PrimaryGunReloadState Enum"))
  (return (`self.CurrentReloadState`)))

(fn `GetNormalizedReloadElapsedTime`
  (returns (ReloadElapsedTime :type "Float (double-precision)"))
  (return (/ (`self.ReloadElapsedTime`) (`self.NormalReloadDuration`))))

(fn `GetNormalizedReloadTimings`
  (returns (PerfectReloadStartTime :type "Float (double-precision)") (ActiveReloadStartTime :type "Float (double-precision)") (ActiveReloadEndTime :type "Float (double-precision)"))
  (bind _normalreloadduration (`self.NormalReloadDuration`))
  (return (/ (`self.PerfectReloadStartTime`) _normalreloadduration) (/ (`self.ActiveReloadStartTime`) _normalreloadduration) (/ (`self.ActiveReloadEndTime`) _normalreloadduration)))

(fn `GetReferences`
  (set `self.CharacterInventory` (`Actor.GetComponentByClass` (`self.GetOwner`) "/Game/0_Design/GameManagement_/BP_InventoryComponent.BP_InventoryComponent_C"))
  (set `self.HUD` (`PlayerController.GetHUD` (`GameplayStatics.GetPlayerController` 0)))
  ;[1 1 1] Get the Gun without any HardReferences
  (for _array_element (`Actor.K2_GetComponentsByClass` (`self.GetOwner`) "/Script/Engine.ChildActorComponent")
    (bind _childactor (`ChildActorComponent.ChildActor` _array_element))
    (if (`/Game/o_Libraries/BPL_GeneralUtilities.Is Actor Of Class` _childactor "/Game/0_Design/GameManagement_/BP_Gun.BP_Gun_C")
      (set `self.CharacterGun` _childactor)
      (break)))
  (bind _maxammocount (message `/Game/0_Design/ReloadSystem/BPI_ReloadSystemGun.GetMaxMagazineAmmoCount` (`self.CharacterGun`)))
  (set `self.MaxMagazineAmmoCount` _maxammocount))

(fn `IsAmmoFull`
  (returns (ReturnValue :type Boolean))
  (bind _currentammocount (message `/Game/0_Design/ReloadSystem/BPI_ReloadSystemGun.GetCurrentMagazineAmmoCount` (`self.CharacterGun`)))
  (return (== _currentammocount (`self.MaxMagazineAmmoCount`))))

(fn `IsGunFireLocked`
  (returns (GunIsLocked :type Boolean))
  (return (`self.IsReloadActive`)))

(fn `On Reload Input`
  (if (`self.IsAmmoFull`)
    (`KismetSystemLibrary.PrintText` "FULL AMMO CALL SCREEN FX OR POST PROCESS")
    (else
      ;[1 1 1 0.33] Do we have ammo in our inventory?
      (if (or (> (`/Game/0_Design/GameManagement_/BP_InventoryComponent.CurrentDefaultAmmoAmount` (`self.CharacterInventory`)) 0) (`self.UseInfiniteAmmo`))
        (switch `/Game/0_Design/ReloadSystem/Enums/E_PrimaryGunState` (`self.CurrentGunState`)
          (:`NewEnumerator0`
            (`self.StartReloadSequence`))
          (:`NewEnumerator2`
            ;[1 1 1] Based on the timing of triggering the reload, we defined if it is a Failed Reload, a Perfect Reload or an Active Reload
            (`KismetSystemLibrary.K2_ClearAndInvalidateTimerHandle` (`self.TimerHandleReloadPlayback`))
            (if (`KismetMathLibrary.InRange_FloatFloat` (`self.ReloadElapsedTime`) (`self.PerfectReloadStartTime`) (`self.ActiveReloadEndTime`))
              (if (< (`self.ReloadElapsedTime`) (`self.ActiveReloadStartTime`))
                (`self.TriggerPerfectReload`)
                (else
                  (`self.TriggerActiveReload`)))
              (else
                (`self.TriggerFailedReload`)))))
        (else
          (`KismetSystemLibrary.PrintText` "Can't reload! We have no ammo in our inventory!!" true true (struct :`R` 1.0 :`B` 0.462642 :`A` 1.0) 5.0))))))

(fn `UpdateAmmoCount`
  (params (NewCount :type Integer))
  (returns (Output_Get :type Integer))
  (message `/Game/0_Design/ReloadSystem/BPI_ReloadSystemGun.SetNewAmmoCount` (`self.CharacterGun`) NewCount)
  (return 0))

(fn `UpdateCurrentReloadState`
  (params (NewState :type "/Game/0_Design/ReloadSystem/Enums/E_PrimaryGunReloadState Enum" :default "NewEnumerator0"))
  (bind _output_get (set `self.CurrentReloadState` NewState))
  (message `/Game/0_Design/ReloadSystem/BPI_ReloadSystemUpdate.UpdateReloadSystemState` (`self.HUD`) _output_get)
  (`self.OnReloadStateUpdated`))