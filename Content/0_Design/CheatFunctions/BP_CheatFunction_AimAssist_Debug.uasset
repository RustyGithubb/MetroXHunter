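; Cheat function that toggles the debug mode of the aim assist component on the player's pawn.
; On init it waits one tick, then caches that component through the cheat manager's player controller and controlled pawn.
; When triggered, and only if the component is enabled, it copies the toggle state to the component's debug flag and calls its HUD initialization.
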(event `self.OnInit`
  (`KismetSystemLibrary.DelayUntilNextTick`)
  (`self.GetReferences`))

(event `self.OnCheat`
  (bind _aimassistcomponent (`self.AimAssistComponent`))
  (if (`/AdvancedAimAssist/Blueprints/Components/AAA_BP_AimAssistComponent.bIsComponentEnable` _aimassistcomponent)
    (set `/AdvancedAimAssist/Blueprints/Components/AAA_BP_AimAssistComponent.bIsDebugActivated` (`self.bIsToggled`) _aimassistcomponent)
    (`/AdvancedAimAssist/Blueprints/Components/AAA_BP_AimAssistComponent.Initialize HUD` _aimassistcomponent)))

(fn `GetReferences`
  (set `self.AimAssistComponent` (`Actor.GetComponentByClass` (`Controller.K2_GetPawn` (`CheatManager.GetPlayerController` (`self.CheatManager`))) "/AdvancedAimAssist/Blueprints/Components/AAA_BP_AimAssistComponent.AAA_BP_AimAssistComponent_C")))