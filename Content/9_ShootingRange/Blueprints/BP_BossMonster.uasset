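; Shooting range boss monster that spins continuously and exposes organ weak points while targeted.
; Targeting swaps its body meshes to an alpha material and enables the weak points with the player camera; untargeting reverts both after a short, cancellable delay.
; Each weak point's death event increments a downed-organ count, advancing the stage when it reaches the current threshold in StagesInfo, with only debug prints as feedback.
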(event `self.ReceiveBeginPlay`
  ;[0.4802 0 0.01596 0.33] BEGINPLAY
  (`parent.ReceiveBeginPlay`)
  ;;[1 1 1 0.33] Bind WeakPoint's LifeComponent Event OnDeath
  (for _array_element (`self.WeakPoints`)
    (add `/Game/0_Design/LifeSystem/BP_LifeComponent.OnDeath` (`/Game/0_Design/EyeVisionSystem/BP_WeakPoints.LifeComponent` _array_element) (delegate `OnWeakPointDown`))))

(event `OnWeakPointDown`
  ;[0.4802 0 0.01596 0.33] BEGINPLAY
  (`self.UpdateCurrentStage`))

(event `self.ReceiveTick`
  (params (DeltaSeconds :type "Float (single-precision)"))
  ;[1 1 1 0.33] ROTATOR
  (`SceneComponent.K2_AddWorldRotation` (`self.DefaultSceneRoot`) (`KismetMathLibrary.MakeRotator` 0.0 0.0 (`self.RotationSpeed`)) false false))

(event `self.OnTargeted`
  (params (IsTargeted :type Boolean) (PlayerCamera :type "CineCameraComponent Object Reference"))
  (bind _head (`self.Head`))
  ;[1 1 1 0.2] ON TARGETED
  (if IsTargeted
    ;;[1 1 1 0.33] Cancel Untargeted Action if the actor is targeted again
    (set `self.CancelUntargeted` true)
    ;;[1 1 1 0.33] Enable / Disable monster's transparency
    (`PrimitiveComponent.SetMaterial` _head 0 "/Game/9_ShootingRange/Materials/MI_FlatColor_Alpha_Brown.MI_FlatColor_Alpha_Brown")
    (`PrimitiveComponent.SetMaterial` (`self.Mouth`) 0 "/Game/9_ShootingRange/Materials/MI_FlatColor_Alpha_Brown.MI_FlatColor_Alpha_Brown")
    (`PrimitiveComponent.SetMaterial` (`self.Body`) 0 "/Game/9_ShootingRange/Materials/MI_FlatColor_Alpha_Brown.MI_FlatColor_Alpha_Brown")
    (`PrimitiveComponent.SetMaterial` (`self.LeftLeg3`) 0 "/Game/9_ShootingRange/Materials/MI_FlatColor_Alpha_Brown.MI_FlatColor_Alpha_Brown")
    (`PrimitiveComponent.SetMaterial` (`self.LeftLeg2`) 0 "/Game/9_ShootingRange/Materials/MI_FlatColor_Alpha_Brown.MI_FlatColor_Alpha_Brown")
    (`PrimitiveComponent.SetMaterial` (`self.LeftLeg`) 0 "/Game/9_ShootingRange/Materials/MI_FlatColor_Alpha_Brown.MI_FlatColor_Alpha_Brown")
    (`PrimitiveComponent.SetMaterial` (`self.RightLeg`) 0 "/Game/9_ShootingRange/Materials/MI_FlatColor_Alpha_Brown.MI_FlatColor_Alpha_Brown")
    (`PrimitiveComponent.SetMaterial` (`self.RightLeg4`) 0 "/Game/9_ShootingRange/Materials/MI_FlatColor_Alpha_Brown.MI_FlatColor_Alpha_Brown")
    (`PrimitiveComponent.SetMaterial` (`self.RightLeg3`) 0 "/Game/9_ShootingRange/Materials/MI_FlatColor_Alpha_Brown.MI_FlatColor_Alpha_Brown")
    (`PrimitiveComponent.SetMaterial` (`self.RightLeg2`) 0 "/Game/9_ShootingRange/Materials/MI_FlatColor_Alpha_Brown.MI_FlatColor_Alpha_Brown")
    (`PrimitiveComponent.SetMaterial` (`self.LeftLeg1`) 0 "/Game/9_ShootingRange/Materials/MI_FlatColor_Alpha_Brown.MI_FlatColor_Alpha_Brown")
    ;;[1 1 1 0.33] Enable WeakPoints
    (for _array_element (`self.WeakPoints`)
      (`/Game/0_Design/EyeVisionSystem/BP_WeakPoints.EnableWeakPoint` _array_element PlayerCamera))
    (else
      ;;[1 1 1 0.33] Check if still Untargeted
      (set `self.CancelUntargeted` false)
      (`KismetSystemLibrary.Delay` 0.5)
      (if (not (`self.CancelUntargeted`))
        (`PrimitiveComponent.SetMaterial` _head 0 "/Game/9_ShootingRange/Materials/MI_FlatColor_Brown.MI_FlatColor_Brown")
        (`PrimitiveComponent.SetMaterial` (`self.Mouth`) 0 "/Game/9_ShootingRange/Materials/MI_FlatColor_Brown.MI_FlatColor_Brown")
        (`PrimitiveComponent.SetMaterial` (`self.Body`) 0 "/Game/9_ShootingRange/Materials/MI_FlatColor_Brown.MI_FlatColor_Brown")
        (`PrimitiveComponent.SetMaterial` (`self.LeftLeg2`) 0 "/Game/9_ShootingRange/Materials/MI_FlatColor_Brown.MI_FlatColor_Brown")
        (`PrimitiveComponent.SetMaterial` (`self.LeftLeg`) 0 "/Game/9_ShootingRange/Materials/MI_FlatColor_Brown.MI_FlatColor_Brown")
        (`PrimitiveComponent.SetMaterial` (`self.RightLeg`) 0 "/Game/9_ShootingRange/Materials/MI_FlatColor_Brown.MI_FlatColor_Brown")
        (`PrimitiveComponent.SetMaterial` (`self.RightLeg4`) 0 "/Game/9_ShootingRange/Materials/MI_FlatColor_Brown.MI_FlatColor_Brown")
        (`PrimitiveComponent.SetMaterial` (`self.RightLeg3`) 0 "/Game/9_ShootingRange/Materials/MI_FlatColor_Brown.MI_FlatColor_Brown")
        (`PrimitiveComponent.SetMaterial` (`self.RightLeg2`) 0 "/Game/9_ShootingRange/Materials/MI_FlatColor_Brown.MI_FlatColor_Brown")
        (`PrimitiveComponent.SetMaterial` (`self.LeftLeg1`) 0 "/Game/9_ShootingRange/Materials/MI_FlatColor_Brown.MI_FlatColor_Brown")
        (`PrimitiveComponent.SetMaterial` (`self.LeftLeg3`) 0 "/Game/9_ShootingRange/Materials/MI_FlatColor_Brown.MI_FlatColor_Brown")
        ;;[1 1 1 0.33] Disable WeakPoints
        (for _array_element_2 (`self.WeakPoints`)
          (`/Game/0_Design/EyeVisionSystem/BP_WeakPoints.DisableWeakPoint` _array_element_2))))))

(fn `UpdateCurrentStage`
  (bind _result (`/Engine/EditorBlueprintResources/StandardMacros.IncrementInt` (`self.OrgansDown`))
    (:`  `
      (if (>= _result (`BlueprintMapLibrary.Map_Find` (`self.StagesInfo`) (`self.CurrentStage`)))
        (`KismetSystemLibrary.PrintString` "Next Boss Stage !" true true (struct :`R` 1.0 :`B` 0.016606 :`A` 1.0))
        (`/Engine/EditorBlueprintResources/StandardMacros.IncrementInt` (`self.CurrentStage`))
        (else
          (`KismetSystemLibrary.PrintString` "Organs HIT !" true true (struct :`G` 0.265401 :`B` 1.0 :`A` 1.0)))))))

(fn `UserConstructionScript`)