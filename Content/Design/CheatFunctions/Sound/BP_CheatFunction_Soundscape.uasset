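; Cheat function that switches the active Soundscape state through the Soundscape subsystem.
; On init it gathers all child gameplay tags of the SoundScape tag, appends one extra entry, and turns their debug strings into the selectable value names.
; On cheat it clears the previously selected tag's state if that tag is valid, sets the state for the chosen index, and stores that index for the next switch.
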(event `self.OnInit`
  (bind _childrentags (`GameplayLibrary.GetAllChildrenGameplayTags` (`BlueprintGameplayTagLibrary.MakeLiteralGameplayTag` (struct :`TagName` "SoundScape"))))
  (bind _output_get (set `self.GameplayTags` _childrentags))
  (`KismetArrayLibrary.Array_Add` _output_get)
  (for _array_element _output_get
    (`KismetArrayLibrary.Array_Add` (`self.ValueNames`) (`BlueprintGameplayTagLibrary.GetDebugStringFromGameplayTag` _array_element))))

(event `self.OnCheat`
  (bind _output (`|GetArrayItem` (`self.GameplayTags`) (`self.LastIndex`)))
  (if (`BlueprintGameplayTagLibrary.IsGameplayTagValid` _output)
    (`SoundscapeSubsystem.ClearState` (subsystem `SoundscapeSubsystem`) _output))
  (`SoundscapeSubsystem.SetState` (subsystem `SoundscapeSubsystem`) (`|GetArrayItem` (`self.GameplayTags`) (`self.Index`)))
  (set `self.LastIndex` (`self.Index`)))