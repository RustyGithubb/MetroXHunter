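; Destructible pipe that leaks steam when shot, as long as it is full of gas.
; Bullet hits passed to TakeDamage leave a decal and call SpawnFX, which adds a Niagara jet, looping sound and damage box along the hit normal.
; Spawn rate and sprite size are divided among active leaks.
; A hit while three leaks are active calls ResetLeaks, clearing them and marking the pipe empty.
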(fn `CanCallTakeDamage`
  (params (DamageContext :type "DamageContext Structure (by ref)"))
  (returns (ReturnValue :type Boolean))
  (return true))

(fn `IsShownAsDamageableToPlayer`
  (params (DamageType :type "EDamageType Enum" :default "Generic") (HitResult :type "HitResult Structure (by ref)"))
  (returns (ReturnValue :type Boolean))
  (return false))

(fn `ResetLeaks`
  (params (ShouldResetState :type Boolean))
  (bind _niagaraleaks (`self.NiagaraLeaks`))
  (bind _boxcollisions (`self.BoxCollisions`))
  (message `AudioParameterControllerInterface.SetTriggerParameter` (`self.SteamSounds`) "Stop_LP")
  (for _array_element _niagaraleaks
    (`ActorComponent.Deactivate` _array_element)
    (for _array_element_2 _boxcollisions
      (`self.K2_DestroyActor` _array_element_2))
    (`KismetArrayLibrary.Array_Clear` _boxcollisions))
  (`KismetArrayLibrary.Array_Clear` _niagaraleaks)
  (set `self.IsGasFull` ShouldResetState))

(fn `SpawnFX`
  (params (Location :type "Vector Structure") (Direction :type "Vector Structure"))
  (locals (SpawnRate :type "Float (single-precision)") (SpriteSizeMin :type "Float (single-precision)") (SpriteSizeMax :type "Float (single-precision)") (DefaultSpawnRate :type "Float (double-precision)" :default 250.0) (DefaultMinSpriteSize :type "Float (double-precision)" :default 75.0) (DefaultMaxSpriteSize :type "Float (double-precision)" :default 100.0))
  (bind _returnvalue (`KismetMathLibrary.Conv_VectorToRotator` Direction))
  (bind _niagaraleaks (`self.NiagaraLeaks`))
  (bind _returnvalue_2 (`KismetArrayLibrary.Array_Length` _niagaraleaks))
  (if (`self.IsGasFull`)
    (if (>= (`KismetArrayLibrary.Array_Length` (`self.NiagaraLeaks`)) 3)
      (`self.ResetLeaks` false)
      (else
        (bind _returnvalue_3 (`|SpawnActorFromClass` "/Game/Design/GPE/BP_DamageBox.BP_DamageBox_C" (`KismetMathLibrary.MakeTransform` (+ Location (* Direction 200.0)) _returnvalue (200.0 40.0 40.0)) "Undefined" "MultiplyWithRoot" null null))
        (`KismetArrayLibrary.Array_Add` (`self.BoxCollisions`) _returnvalue_3)
        (bind _returnvalue_4 (`NiagaraFunctionLibrary.SpawnSystemAtLocation` (`self.SteamVFX`) Location _returnvalue))
        (`AudioComponent.SetSound` (`self.SteamSounds`) "/Game/Sounds/Audio/SD/MetaSounds/MS_Sources/GPE/Pipe_Steam/MS_Steam_Full.MS_Steam_Full") ; NOTE: The sound asset must have "Looping" set to true
        (`AudioComponent.Play` (`self.SteamSounds`) 0.0)
        (`KismetArrayLibrary.Array_Add` _niagaraleaks _returnvalue_4)
        (set `local.SpawnRate` (/ (`local.DefaultSpawnRate`) _returnvalue_2))
        (set `local.SpriteSizeMin` (/ (`local.DefaultMinSpriteSize`) _returnvalue_2))
        (set `local.SpriteSizeMax` (/ (`local.DefaultMaxSpriteSize`) _returnvalue_2))
        (for _array_element (`self.NiagaraLeaks`)
          (`FXSystemComponent.SetFloatParameter` _array_element "SpawnRate" (`local.SpawnRate`))
          (`FXSystemComponent.SetFloatParameter` _array_element "SpriteSizeMin" (`local.SpriteSizeMin`))
          (`FXSystemComponent.SetFloatParameter` _array_element "SpriteSizeMax" (`local.SpriteSizeMax`)))))))

(fn `TakeDamage`
  (params (DamageContext :type "DamageContext Structure (by ref)"))
  (returns (ReturnValue :type Boolean))
  (bind (_healthcomponent _damageamount _damagetype _attackeractor _inflictoractor _hitresult) (break `DamageContext` DamageContext))
  (bind (_bblockinghit _binitialoverlap _time _distance _location _impactpoint _normal) (`GameplayStatics.BreakHitResult` _hitresult))
  (if (`|EnumEquality` _damagetype "Bullet")
    (bind _returnvalue (`|SpawnActorFromClass` "/Game/Art/VFX/GPE/Decal/BP_Bullet_Decals.BP_Bullet_Decals_C" (`KismetMathLibrary.MakeTransform` _location (`KismetMathLibrary.Conv_VectorToRotator` _normal) (0.05 0.05 0.05)) "AlwaysSpawn" "MultiplyWithRoot" null null))
    (`/Game/Art/VFX/GPE/Decal/BP_Bullet_Decals.StartDecal` _returnvalue false)
    (`self.SpawnFX` _location _normal)
    (return false)))

(fn `UserConstructionScript`)