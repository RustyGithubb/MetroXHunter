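; Actor component that plays the audio for BP_ZeroEnemy, the big monster enemy.
; It binds to damage, death and state updates, and exposes events for gore, knockout, revival and rush scream, mostly playing sounds attached to the mesh.
; Death sound follows a random delay.
; The Rush Attack Resolve state plays 2D QTE grab and loop sounds, fades the loop on exit, and plays success or failure stingers.
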(event `self.ReceiveBeginPlay`
  (bind _healthcomponent (`ZeroEnemy.HealthComponent` (`self.ZeroEnemy`)))
  (bind _asbp_zero_enemy (cast `/Game/Design/Enemies/AI/Zero/BP_ZeroEnemy` (`self.GetOwner`)))
  (set `self.ZeroEnemy` _asbp_zero_enemy)
  (add `HealthComponent.OnDamage` _healthcomponent (`|CreateDelegate` :!event `OnDamage`))
  (add `HealthComponent.OnDeath` _healthcomponent (`|CreateDelegate` :!event `OnDeath`))
  (add `ZeroEnemy.OnStateUpdate` (`self.ZeroEnemy`) (`|CreateDelegate` :!event `OnStateUpdate`)))

(event `self.OnBulbDestroy`
  (params (HitResult :type "HitResult Structure (by ref)"))
  ;[1 0 0 0.33 32] GORE
  (`GameplayStatics.SpawnSoundAttached` "/Game/Sounds/Audio/SD/MetaSounds/MS_Sources/Ennemies/BigMonster/MS_BigMonster_Gore.MS_BigMonster_Gore" (`Character.Mesh` (`self.ZeroEnemy`)) "None" (0.0 0.0 0.0) (struct) "KeepWorldPosition" true 1.0 1.0 0.0 null null))

(event `OnDamage`
  (params (DamageContext :type "DamageContext Structure (by ref)"))
  ;[1 0 0 0.33 32] DAMAGE
  (`GameplayStatics.SpawnSoundAttached` "/Game/Sounds/Audio/SD/MetaSounds/MS_Sources/Ennemies/BigMonster/MS_BigMonster_Damage.MS_BigMonster_Damage" (`Character.Mesh` (`self.ZeroEnemy`)) "None" (0.0 0.0 0.0) (struct) "KeepRelativeOffset" false 1.0 1.0 0.0 null null))

(event `self.OnLegDestroy`
  (params (SkeletalMeshComponent :type "SkeletalMeshComponent Object Reference") (BoneName :type "Name (by ref)") (HitLocation :type "Vector Structure (by ref)"))
  ;[1 0 0 0.33 32] GORE
  (`GameplayStatics.SpawnSoundAttached` "/Game/Sounds/Audio/SD/MetaSounds/MS_Sources/Ennemies/BigMonster/MS_BigMonster_Gore.MS_BigMonster_Gore" SkeletalMeshComponent BoneName HitLocation (struct) "KeepWorldPosition" true 1.0 1.0 0.0 null null))

(event `OnDeath`
  (params (DamageContext :type "DamageContext Structure (by ref)"))
  ;[1 0 0 0.33 32] DAMAGE
  (`KismetSystemLibrary.Delay` (`KismetMathLibrary.RandomFloatInRange` 2.0 4.0))
  (`GameplayStatics.SpawnSoundAttached` "/Game/Sounds/Audio/SD/MetaSounds/MS_Sources/Ennemies/BigMonster/MS_BigMonster_Death.MS_BigMonster_Death" (`Character.Mesh` (`self.ZeroEnemy`)) "None" (0.0 0.0 0.0) (struct) "KeepRelativeOffset" false 1.0 1.0 0.0 null null))

(event `self.OnLimbDestroy`
  (params (SkeletalMeshComponent :type "SkeletalMeshComponent Object Reference") (BoneName :type "Name (by ref)") (HitLocation :type "Vector Structure (by ref)"))
  ;[1 0 0 0.33 32] GORE
  (`GameplayStatics.SpawnSoundAttached` "/Game/Sounds/Audio/SD/MetaSounds/MS_Sources/Ennemies/BigMonster/MS_BigMonster_Gore.MS_BigMonster_Gore" SkeletalMeshComponent BoneName HitLocation (struct) "KeepWorldPosition" true 1.0 1.0 0.0 null null))

(event `self.OnKnockedOut`
  ;[0 1 0.8457 0.33 32] STATES
  (`GameplayStatics.SpawnSoundAttached` "/Game/Sounds/Audio/SD/MetaSounds/MS_Sources/Ennemies/BigMonster/MS_BigMonster_Damage.MS_BigMonster_Damage" (`Character.Mesh` (`self.ZeroEnemy`)) "None" (0.0 0.0 0.0) (struct) "KeepRelativeOffset" false 1.0 1.0 0.0 null null))

(event `self.OnRevival`
  ;[0 1 0.8457 0.33 32] STATES
  (`GameplayStatics.SpawnSoundAttached` "/Game/Sounds/Audio/SD/MetaSounds/MS_Sources/Ennemies/BigMonster/MS_BigMonster_Revival.MS_BigMonster_Revival" (`Character.Mesh` (`self.ZeroEnemy`)) "None" (0.0 0.0 0.0) (struct) "KeepRelativeOffset" false 1.0 1.0 0.0 null null))

(event `self.OnRushScream`
  ;[0 1 0.8457 0.33 32] STATES
  (`GameplayStatics.SpawnSoundAttached` "/Game/Sounds/Audio/SD/SoundWaves/Enemies/QTE_BigMonster/SW_QTE_BigMonster_Rush.SW_QTE_BigMonster_Rush" (`Character.Mesh` (`self.ZeroEnemy`)) "None" (0.0 0.0 0.0) (struct) "KeepRelativeOffset" false 1.0 1.0 0.0 null null))

(event `OnStateUpdate`
  (params (NewState :type "EZeroEnemyState Enum" :default "None") (OldState :type "EZeroEnemyState Enum" :default "None"))
  ;[0 1 0.8457 0.33 32] STATES
  (`|ExecutionSequence`
    (:`then_0`
      (switch `EZeroEnemyState` NewState
        (:`RushAttackResolve`
          ;;[0 1 0.3805 0.33 32] QTE
          (bind _returnvalue (`GameplayStatics.SpawnSound2D` "/Game/Sounds/Audio/SD/SoundWaves/Enemies/QTE_BigMonster/SW_QTE_BigMonster_LP.SW_QTE_BigMonster_LP" 1.0 1.0 0.0 null)) ; Loop sound
          (set `self.SoundQTE` _returnvalue)
          (`GameplayStatics.PlaySound2D` "/Game/Sounds/Audio/SD/SoundWaves/Enemies/QTE_BigMonster/SW_QTE_BigMonster_Grab.SW_QTE_BigMonster_Grab" 1.0 1.0 0.0 null null) ; Grab sound
          (add `QuickTimeEventComponent.OnEventStopped` (`/Game/Design/Enemies/AI/Zero/BP_ZeroEnemy.EnemyQuickTimeEventComponent` (`self.ZeroEnemy`)) (delegate `OnEventStopped_Event`)))))
    (:`then_1`
      (switch `EZeroEnemyState` OldState
        (:`RushAttackResolve`
          (bind _soundqte (`self.SoundQTE`)
            (:`then`
              (`AudioComponent.FadeOut` _soundqte 0.5 0.0 "Linear") ; Fade out loop sound
            )
            (:`else`)))))))

(event `OnEventStopped_Event`
  (params (Component :type "QuickTimeEventComponent Object Reference") (DataAsset :type "QuickTimeEventData Object Reference") (EventResult :type "EQuickTimeEventResult Enum" :default "Succeed"))
  ;[0 1 0.8457 0.33 32] STATES
  ;;[0 1 0.3805 0.33 32] QTE
  (remove `QuickTimeEventComponent.OnEventStopped` (`/Game/Design/Enemies/AI/Zero/BP_ZeroEnemy.EnemyQuickTimeEventComponent` (`self.ZeroEnemy`)) (delegate `OnEventStopped_Event`))
  (switch `EQuickTimeEventResult` EventResult
    (:`Succeed`
      (`GameplayStatics.PlaySound2D` (`KismetArrayLibrary.Array_Random` (`|MakeArray` "/Game/Sounds/Audio/SD/SoundWaves/Enemies/QTE_BigMonster/SW_QTE_BigMonster_Success_01.SW_QTE_BigMonster_Success_01" "/Game/Sounds/Audio/SD/SoundWaves/Enemies/QTE_BigMonster/SW_QTE_BigMonster_Success_02.SW_QTE_BigMonster_Success_02" :!type "SoundBase Object Reference")) 1.0 1.0 0.0 null null) ; Success sound
    )
    (:`Failed`
      (`GameplayStatics.PlaySound2D` "/Game/Sounds/Audio/SD/SoundWaves/Enemies/QTE_BigMonster/SW_QTE_BigMonster_Death.SW_QTE_BigMonster_Death" 1.0 1.0 0.0 null null) ; Failed sound
    )))