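; Animated coil (bobine) that displays the state of the player's BP_Gun, lighting up in Lightning mode and shutting down in Bullet mode.
; Gun delegates handle weapon switches and lightning end, driving a fuse, six energy-threshold lamps and a startup spin boost.
; Tick eases coil rotation toward a charge-based target and updates lamps when their count changes.
; Timelines fade flickering emissive on dynamic materials; the heat-distortion effect is unconnected.
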(event `self.ReceiveBeginPlay`
  ;[1 0 0 0.33 50] event begin play
  (bind _asbp_main_chara (cast `/Game/Design/_GameManagement/BP_MainChara` (`GameplayStatics.GetPlayerCharacter` 0)))
  (set `self.Player Character` _asbp_main_chara)
  (bind _asbp_gun (cast `/Game/Design/_GameManagement/BP_Gun` (`ChildActorComponent.ChildActor` (`/Game/Design/_GameManagement/BP_MainChara.Weapon` _asbp_main_chara))))
  (set `self.Gun Reference` _asbp_gun)
  (`|ExecutionSequence`
    (:`then_0`
      (`self.Create all dynamic material`)
      (set `self.LampArray` (`|MakeArray` (`self.lamp_6`) (`self.lamp_5`) (`self.lamp_4`) (`self.lamp_3`) (`self.lamp_2`) (`self.lamp_1`) (`self.fuse`))))
    (:`then_1`
      (`self.BindToDelegates`)
      (`self.OnWeaponSwitch` "Bullet"))))

(event `UpdateTargetRotation`
  (bind _gun_reference (`self.Gun Reference`))
  (set `self.Target Rotation` (`KismetMathLibrary.FInterpTo` (`self.Target Rotation`) (+ (* (* (`/Game/Design/_GameManagement/BP_Gun.LightningChargeValue` _gun_reference) 3.0) (* (`/Game/Design/_GameManagement/BP_Gun.ChargingWeight` _gun_reference) 3.0)) (`self.Addon Allumage`)) (`GameplayStatics.GetWorldDeltaSeconds`) 100.0)))

(event `OnEndLightning`
  (set `self.Target Rotation` (`self.Addon Allumage`)))

(event `OnWeaponSwitch`
  (params (Selection :type "EGunMode Enum" :default "Bullet"))
  (switch `EGunMode` Selection
    (:`Bullet`
      ;[1 1 1 0.33] Turn off fuse & lamps
      (set `self.IsLampOn` false)
      (`self.SwitchFuse` false)
      (`self.SwitchOffAllLamps`)
      (set `self.Target Rotation` 0.0))
    (:`Lightning`
      ;[1 1 1 0.33] Turn on fuse & update lamps
      (set `self.IsLampOn` true)
      (`self.AddonAllumage`)
      (`self.SwitchFuse` true)
      (set `self.EnergyRatio` (`self.CalculateEnergyRatio`))
      (bind _targetcount (`self.GetTargetLampOn`))
      (`self.SwitchOnLamps` _targetcount))))

(event `self.ReceiveTick`
  (params (DeltaSeconds :type "Float (single-precision)"))
  (`|ExecutionSequence`
    (:`then_0`
      ;[0 0 0 1 50] ROTATION WHEN USE
      (bind _output_get (set `self.Rotation Bobine Value` (`KismetMathLibrary.FInterpTo` (`self.Rotation Bobine Value`) (`self.Target Rotation`) (`GameplayStatics.GetWorldDeltaSeconds`) 2.0)))
      (`SceneComponent.K2_AddLocalRotation` (`self.PH_Bobine_Socle`) (`KismetMathLibrary.MakeRotator` 0.0 _output_get) false false))
    (:`then_1`
      (if (`self.IsLampOn`)
        (`self.UpdateTargetRotation`)
        ;[1 1 1 0.33] Get Energy Ratio
        (set `self.EnergyRatio` (`self.CalculateEnergyRatio`))
        ;[1 1 1 0.33] Update ON/OFF lamps
        (bind _targetcount (`self.GetTargetLampOn`))
        (bind _output_get_2 (set `self.Target Count` _targetcount))
        (if (not (== _output_get_2 (`self.CurrentLampOn`)))
          (bind _output_get_3 (set `self.CurrentLampOn` (`self.Target Count`)))
          (`self.UpdateLamps` _output_get_3))))))

(event `SwitchLampOne`
  (params (IsOn :type Boolean))
  ;[0 0 0 0.33 100] SWITCH MODE LAMP
  (if IsOn
    (bind (_direction _c_bobine_swithmode) (`Timeline|Timeline` :!label _label)
      (:`Update`
        (`MaterialInstanceDynamic.SetScalarParameterValue` (`|GetArrayItem` (`self.LampArray`)) "Emissive" (* _c_bobine_swithmode (`self.Light On`) (`KismetMathLibrary.RandomFloatInRange` (`self.Min`) (`self.Max`))))))
    (else
      (goto _label :!via `Reverse`))))

(event `SwitchLampTwo`
  (params (IsOn :type Boolean))
  ;[0 0 0 0.33 100] SWITCH MODE LAMP
  (if IsOn
    (bind (_direction _c_bobine_swithmode) (`Timeline|Timeline_0` :!label _label_2)
      (:`Update`
        (`MaterialInstanceDynamic.SetScalarParameterValue` (`|GetArrayItem` (`self.LampArray`) 1) "Emissive" (* _c_bobine_swithmode (`self.Light On`) (`KismetMathLibrary.RandomFloatInRange` (`self.Min`) (`self.Max`))))))
    (else
      (goto _label_2 :!via `Reverse`))))

(event `SwitchLampThree`
  (params (IsOn :type Boolean))
  ;[0 0 0 0.33 100] SWITCH MODE LAMP
  (if IsOn
    (bind (_direction _c_bobine_swithmode) (`Timeline|Timeline_1` :!label _label_3)
      (:`Update`
        (`MaterialInstanceDynamic.SetScalarParameterValue` (`|GetArrayItem` (`self.LampArray`) 2) "Emissive" (* _c_bobine_swithmode (`self.Light On`) (`KismetMathLibrary.RandomFloatInRange` (`self.Min`) (`self.Max`))))))
    (else
      (goto _label_3 :!via `Reverse`))))

(event `SwitchLampFour`
  (params (IsOn :type Boolean))
  ;[0 0 0 0.33 100] SWITCH MODE LAMP
  (if IsOn
    (bind (_direction _c_bobine_swithmode) (`Timeline|Timeline_2` :!label _label_4)
      (:`Update`
        (`MaterialInstanceDynamic.SetScalarParameterValue` (`|GetArrayItem` (`self.LampArray`) 3) "Emissive" (* _c_bobine_swithmode (`self.Light On`) (`KismetMathLibrary.RandomFloatInRange` (`self.Min`) (`self.Max`))))))
    (else
      (goto _label_4 :!via `Reverse`))))

(event `SwitchLampFive`
  (params (IsOn :type Boolean))
  ;[0 0 0 0.33 100] SWITCH MODE LAMP
  (if IsOn
    (bind (_direction _c_bobine_swithmode) (`Timeline|Timeline_3` :!label _label_5)
      (:`Update`
        (`MaterialInstanceDynamic.SetScalarParameterValue` (`|GetArrayItem` (`self.LampArray`) 4) "Emissive" (* _c_bobine_swithmode (`self.Light On`) (`KismetMathLibrary.RandomFloatInRange` (`self.Min`) (`self.Max`))))))
    (else
      (goto _label_5 :!via `Reverse`))))

(event `SwitchLampSix`
  (params (IsOn :type Boolean))
  ;[0 0 0 0.33 100] SWITCH MODE LAMP
  (if IsOn
    (bind (_direction _c_bobine_swithmode) (`Timeline|Timeline_4` :!label _label_6)
      (:`Update`
        (`MaterialInstanceDynamic.SetScalarParameterValue` (`|GetArrayItem` (`self.LampArray`) 5) "Emissive" (* _c_bobine_swithmode (`self.Light On`) (`KismetMathLibrary.RandomFloatInRange` (`self.Min`) (`self.Max`))))))
    (else
      (goto _label_6 :!via `Reverse`))))

(event `SwitchFuse`
  (params (IsOn :type Boolean))
  ;[0 0 0 0.33 100] SWITCH MODE LAMP
  (if IsOn
    (bind (_direction _c_bobine_swithmode) (`Timeline|Timeline_6` :!label _label_7)
      (:`Update`
        (`MaterialInstanceDynamic.SetScalarParameterValue` (`|GetArrayItem` (`self.LampArray`) 6) "Emissive" (* _c_bobine_swithmode (`self.Light On`) (`KismetMathLibrary.RandomFloatInRange` (`self.Min`) (`self.Max`))))))
    (else
      (goto _label_7 :!via `Reverse`))))

(event `AddonAllumage`
  ;[0 0 0 0.33 100] SWITCH MODE LAMP
  (bind (_direction _c_bobine_swithmode_start) (`Timeline|Timeline_5` :!via `PlayFromStart`)
    (:`Update`
      (bind _output_get (set `self.Addon Allumage` (* _c_bobine_swithmode_start (`self.RotationSartStrength`))))
      (set `self.Target Rotation` _output_get))
    (:`Finished`
      (if (not (`self.IsLampOn`))
        (set `self.Target Rotation` 0.0)))))

(fn `BindToDelegates`
  (bind _gun_reference (`self.Gun Reference`))
  (add `/Game/Design/_GameManagement/BP_Gun.OnLightningEndEvent` _gun_reference (`|CreateDelegate` :!event `OnEndLightning`))
  (add `/Game/Design/_GameManagement/BP_Gun.OnSwitchWeapon` _gun_reference (`|CreateDelegate` :!event `OnWeaponSwitch`)))

(fn `Create all dynamic material`
  (bind _returnvalue (`PrimitiveComponent.CreateDynamicMaterialInstance` (`self.PH_Bobine_Socle`) 3 null "None")) ; NOTE: The material indices don't make any sense but let's go
  (set `self.lamp_1` _returnvalue)
  (bind _returnvalue_2 (`PrimitiveComponent.CreateDynamicMaterialInstance` (`self.PH_Bobine_Socle`) 2 null "None"))
  (set `self.lamp_2` _returnvalue_2)
  (bind _returnvalue_3 (`PrimitiveComponent.CreateDynamicMaterialInstance` (`self.PH_Bobine_Socle`) 6 null "None"))
  (set `self.lamp_3` _returnvalue_3)
  (bind _returnvalue_4 (`PrimitiveComponent.CreateDynamicMaterialInstance` (`self.PH_Bobine_Socle`) 1 null "None"))
  (set `self.lamp_4` _returnvalue_4)
  (bind _returnvalue_5 (`PrimitiveComponent.CreateDynamicMaterialInstance` (`self.PH_Bobine_Socle`) 5 null "None"))
  (set `self.lamp_5` _returnvalue_5)
  (bind _returnvalue_6 (`PrimitiveComponent.CreateDynamicMaterialInstance` (`self.PH_Bobine_Socle`) 4 null "None"))
  (set `self.lamp_6` _returnvalue_6)
  (bind _returnvalue_7 (`PrimitiveComponent.CreateDynamicMaterialInstance` (`self.PH_Bobine_base`) 1 null "None"))
  (set `self.fuse` _returnvalue_7))

(fn `GetTargetLampOn`
  (returns (TargetCount :type Integer))
  (locals (TargetLampOn :type Integer))
  (`|ExecutionSequence`
    (:`then_0`
      (if (>= (`self.EnergyRatio`) 0.83)
        (set `local.TargetLampOn` 6)
        (elif (>= (`self.EnergyRatio`) 0.66)
          (set `local.TargetLampOn` 5)
          (elif (>= (`self.EnergyRatio`) 0.5)
            (set `local.TargetLampOn` 4)
            (elif (>= (`self.EnergyRatio`) 0.33)
              (set `local.TargetLampOn` 3)
              (elif (>= (`self.EnergyRatio`) 0.16)
                (set `local.TargetLampOn` 2)
                (elif (> (`self.EnergyRatio`) 0.075)
                  (set `local.TargetLampOn` 1)
                  (else
                    (set `local.TargetLampOn` 0)))))))))
    (:`then_1`
      (return (`local.TargetLampOn`)))))

(fn `SwitchOffAllLamps`
  (`self.SwitchLampSix` false)
  (`self.SwitchLampFive` false)
  (`self.SwitchLampFour` false)
  (`self.SwitchLampThree` false)
  (`self.SwitchLampTwo` false)
  (`self.SwitchLampOne` false))

(fn `SwitchOnLamps`
  (params (LampCount :type Integer))
  (if (not (< LampCount 1))
    (`self.SwitchLampSix` true)
    (if (not (< LampCount 2))
      (`self.SwitchLampFive` true)
      (if (not (< LampCount 3))
        (`self.SwitchLampFour` true)
        (if (not (< LampCount 4))
          (`self.SwitchLampThree` true)
          (if (not (< LampCount 5))
            (`self.SwitchLampTwo` true)
            (if (not (< LampCount 6))
              (`self.SwitchLampOne` true))))))))

(fn `UpdateLamps`
  (params (Selection :type Integer))
  (switch `int` Selection
    (:`0`
      (`self.SwitchLampSix` false))
    (:`1`
      (`self.SwitchLampFive` false)
      (`self.SwitchLampSix` true))
    (:`2`
      (`self.SwitchLampFour` false)
      (`self.SwitchLampFive` true))
    (:`3`
      (`self.SwitchLampThree` false)
      (`self.SwitchLampFour` true))
    (:`4`
      (`self.SwitchLampTwo` false)
      (`self.SwitchLampThree` true))
    (:`5`
      (`self.SwitchLampOne` false)
      (`self.SwitchLampTwo` true))
    (:`6`
      (`self.SwitchLampOne` true))))

(fn `UserConstructionScript`)