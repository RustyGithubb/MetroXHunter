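; Actor component that tracks integer life and death state for its owner.
; It starts at MaxLife and lowers CurrentLife through TakeDamage, skipped while invulnerable or dead, firing health update, damage and, at zero or below, death dispatchers with the damage context.
; Heal clamps life to MaxLife and can revive from death, while ResetLife restores full life and clears the dead flag.
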(event `self.ReceiveBeginPlay`
  ;[1 0 0.01418 0.33] BEGINPLAY
  ;;[0 1 0.4761] Set CurrentLife
  (set `self.CurrentLife` (`self.MaxLife`)))

(fn `Heal`
  (params (HealAmount :type Integer))
  (set `self.CurrentLife` (`KismetMathLibrary.Clamp` (+ (`self.CurrentLife`) HealAmount) 0 (`self.MaxLife`)))
  ;[1 1 1 0.33] Reset death
  (if (and (`self.IsDead`) (> (`self.CurrentLife`) 0))
    (set `self.IsDead` false))
  (`self.OnHealthUpdate`))

(fn `ResetLife`
  (set `self.CurrentLife` (`self.MaxLife`))
  (set `self.IsDead` false)
  (`self.OnHealthUpdate`))

(fn `TakeDamage`
  (params (DamageContext :type "/Game/Design/LifeSystem/Structs/F_DamageContext Structure"))
  (bind _damagecontext (`local.DamageContext`))
  (if (not (`self.isInvulnerable`))
    (if (not (`self.IsDead`))
      ;[1 1 1 0.33] Apply damage to health
      (set `self.CurrentLife` (- (`self.CurrentLife`) (`.DamageAmount_2_F15E80544E9AA4927A1CD79E00C5FD10` (break `/Game/Design/LifeSystem/Structs/F_DamageContext` DamageContext))))
      (`self.OnHealthUpdate`)
      (`self.OnDamage` _damagecontext)
      ;[0 1 0.6778] Call OnDeath event
      (if (<= (`self.CurrentLife`) 0)
        (set `self.IsDead` true)
        (`self.OnDeath` _damagecontext)))))