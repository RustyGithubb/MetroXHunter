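; Trigger receiver component that teleports the player between two trigger boxes when a component-specific event fires.
; The event cannot identify its source box, so the component compares distances and moves the player to the farther one.
; A short timer-based cooldown blocks the instant re-trigger from arriving in the destination box.
; BeginPlay enables teleporting only if both boxes are valid, otherwise it prints a warning naming the owner.
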(event `self.ReceiveBeginPlay`
  (set `self.PlayerCharacter` (`GameplayStatics.GetPlayerPawn` 0))
  (`self.TriggerBox01`
    (:`then`
      (`self.TriggerBox02`
        (:`then`
          (set `self.AllowTP` true))
        (:`else`
          (`KismetSystemLibrary.PrintText` (`|FormatText` "TeleporterTriggerComponent on Actor {Actor} doesn't have target TriggerBoxes for Teleporting! \nPlease add some!!" (`self.GetOwner`)) :!label _label))))
    (:`else`
      (goto _label))))

(event `ReAllowTP`
  (set `self.AllowTP` true))

(fn `OnPlayComponentSpecificEvent`
  (params (FromBoxEnter :type Boolean))
  (if (`self.AllowTP`)
    ;[1 1 1 0.33] Block TP for a time to prevent infinite Teleportation
    ; When we move the Player it activates the next Triggerbox' TriggerEnter, so we put a cooldown to ignore the instant call
    (`KismetSystemLibrary.K2_SetTimerDelegate` (`|CreateDelegate` :!event `ReAllowTP`) 0.3)
    (set `self.AllowTP` false)
    ;[0 0 0 0.33] We have no way of knowing which TriggerBox sends the data, since it's not designed to be called by multiple triggerboxes...
    ; So we'll do a simple distance check and TP to the other one
    (if (> (`Actor.GetDistanceTo` (`self.PlayerCharacter`) (`self.TriggerBox01`)) (`Actor.GetDistanceTo` (`self.PlayerCharacter`) (`self.TriggerBox02`)))
      (`Actor.K2_SetActorLocation` (`self.PlayerCharacter`) (`Actor.K2_GetActorLocation` (`self.TriggerBox01`)) false false)
      (else
        (`Actor.K2_SetActorLocation` (`self.PlayerCharacter`) (`Actor.K2_GetActorLocation` (`self.TriggerBox02`)) false false)))))