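; BP_SettingUnit_ReticleColor is a settings unit that sets the color of the shooting reticle from a preset list.
; When the setting is applied in game, it tints the cursor widget's circle with the preset at the selected index.
; If no widget reference is cached, it only caches the first WBP_CursorShoot found, leaving the color unchanged until the next apply.
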(event `self.OnApplySetting`
  (params (bInGame :type Boolean))
  (bind _wbp_cursorshoot (`self.WBP_CursorShoot`))
  (if bInGame
    (`/Engine/EditorBlueprintResources/StandardMacros.IsValid` _wbp_cursorshoot
      (:`Is Valid`
        (set `Image.ColorAndOpacity` (`|GetArrayItem` (`self.ColorsPreset`) (`self.IndexValue`)) (`/Game/Design/Widgets/WBP_CursorShoot.CircleCursor` _wbp_cursorshoot)))
      (:`Is Not Valid`
        (bind _foundwidgets (`WidgetBlueprintLibrary.GetAllWidgetsOfClass` "/Game/Design/Widgets/WBP_CursorShoot.WBP_CursorShoot_C" false))
        (set `self.WBP_CursorShoot` (`|GetArrayItem` _foundwidgets))))))