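; BP_Tunnel5m is a modular metro tunnel piece, apparently 5 m long, with walls, ceiling, tracks, cables and neon lights.
; Its construction script applies one intensity in candelas to both rect lights, then uses boolean options to cut the ceiling or either half and drop tracks, cables or lights.
; Removed parts are hidden rather than destroyed, with mesh collision also disabled except when only the lights are dropped.
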(fn `UserConstructionScript`
  (bind _sm_r_wall_8 (`self.SM_R_Wall_8`))
  (bind _sm_ceiling (`self.SM_Ceiling`))
  (bind _sm_l_wall_5 (`self.SM_L_Wall_5`))
  (bind _sm_r_cable (`self.SM_R_Cable`))
  (bind _sm_l_1track (`self.SM_L_1Track`))
  ;[1 1 1 0.33] Set Light Intensity
  ;;[1 1 1 0.33] In Candelas
  (`LightComponent.SetIntensity` (`self.R_RectLight`) (`self.IntensityLight`))
  (`LightComponent.SetIntensity` (`self.L_RectLight`) (`self.IntensityLight`))
  (if (`self.CutCeiling`)
    (`SceneComponent.SetVisibility` _sm_ceiling false false)
    (`PrimitiveComponent.SetCollisionEnabled` _sm_ceiling "NoCollision"))
  (if (`self.CutLeftHalf?`)
    (`SceneComponent.SetVisibility` _sm_r_wall_8 false false)
    (`SceneComponent.SetVisibility` (`self.SM_R_Wall_9`) false false)
    (`SceneComponent.SetVisibility` (`self.SM_R_Wall_10`) false false)
    (`SceneComponent.SetVisibility` (`self.SM_R_Wall_2`) false false)
    (`SceneComponent.SetVisibility` (`self.SM_R_Wall_1`) false false)
    (`SceneComponent.SetVisibility` (`self.SM_R_Cable`) false false)
    (`SceneComponent.SetVisibility` (`self.SM_L_Neon`) false false)
    (`SceneComponent.SetVisibility` (`self.L_RectLight`) false false)
    (`PrimitiveComponent.SetCollisionEnabled` _sm_r_wall_8 "NoCollision")
    (`PrimitiveComponent.SetCollisionEnabled` (`self.SM_R_Wall_9`) "NoCollision")
    (`PrimitiveComponent.SetCollisionEnabled` (`self.SM_R_Wall_10`) "NoCollision")
    (`PrimitiveComponent.SetCollisionEnabled` (`self.SM_R_Wall_2`) "NoCollision")
    (`PrimitiveComponent.SetCollisionEnabled` (`self.SM_R_Wall_1`) "NoCollision")
    (`PrimitiveComponent.SetCollisionEnabled` (`self.SM_R_Cable`) "NoCollision")
    (`PrimitiveComponent.SetCollisionEnabled` (`self.SM_L_Neon`) "NoCollision"))
  (if (`self.CutRightHalf?`)
    (`SceneComponent.SetVisibility` _sm_l_wall_5 false false)
    (`SceneComponent.SetVisibility` (`self.SM_L_Wall_11`) false false)
    (`SceneComponent.SetVisibility` (`self.SM_L_Wall_6`) false false)
    (`SceneComponent.SetVisibility` (`self.SM_L_Cable`) false false)
    (`SceneComponent.SetVisibility` (`self.SM_L_Wall_0`) false false)
    (`SceneComponent.SetVisibility` (`self.SM_L_Wall_4`) false false)
    (`SceneComponent.SetVisibility` (`self.SM_R_Neon`) false false)
    (`SceneComponent.SetVisibility` (`self.R_RectLight`) false false)
    (`PrimitiveComponent.SetCollisionEnabled` _sm_l_wall_5 "NoCollision")
    (`PrimitiveComponent.SetCollisionEnabled` (`self.SM_L_Wall_11`) "NoCollision")
    (`PrimitiveComponent.SetCollisionEnabled` (`self.SM_L_Wall_6`) "NoCollision")
    (`PrimitiveComponent.SetCollisionEnabled` (`self.SM_L_Cable`) "NoCollision")
    (`PrimitiveComponent.SetCollisionEnabled` (`self.SM_L_Wall_0`) "NoCollision")
    (`PrimitiveComponent.SetCollisionEnabled` (`self.SM_L_Wall_4`) "NoCollision")
    (`PrimitiveComponent.SetCollisionEnabled` (`self.SM_R_Neon`) "NoCollision"))
  (if (`self.WithoutTracks?`)
    (`SceneComponent.SetVisibility` _sm_l_1track false false)
    (`SceneComponent.SetVisibility` (`self.SM_L_2Track`) false false)
    (`SceneComponent.SetVisibility` (`self.SM_R_1Track`) false false)
    (`SceneComponent.SetVisibility` (`self.SM_R_2Track`) false false)
    (`PrimitiveComponent.SetCollisionEnabled` _sm_l_1track "NoCollision")
    (`PrimitiveComponent.SetCollisionEnabled` (`self.SM_L_2Track`) "NoCollision")
    (`PrimitiveComponent.SetCollisionEnabled` (`self.SM_R_1Track`) "NoCollision")
    (`PrimitiveComponent.SetCollisionEnabled` (`self.SM_R_2Track`) "NoCollision"))
  (if (`self.WithoutCables?`)
    (`SceneComponent.SetVisibility` _sm_r_cable false false)
    (`SceneComponent.SetVisibility` (`self.SM_L_Cable`) false false)
    (`PrimitiveComponent.SetCollisionEnabled` _sm_r_cable "NoCollision")
    (`PrimitiveComponent.SetCollisionEnabled` (`self.SM_L_Cable`) "NoCollision"))
  (if (`self.WithoutLights?`)
    (`SceneComponent.SetVisibility` (`self.SM_R_Neon`) false false)
    (`SceneComponent.SetVisibility` (`self.R_RectLight`) false false)
    (`SceneComponent.SetVisibility` (`self.L_RectLight`) false false)
    (`SceneComponent.SetVisibility` (`self.SM_L_Neon`) false false)))