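; BP_CratePiece is a physics debris piece for a destructible crate that flies off and disappears after a short time.
; On BeginPlay it picks a random lifetime and starting scale, then applies an impulse of random strength along its ImpulseDirection.
; Tick counts the lifetime down, shrinks the piece in proportion to the time left during the final second, then destroys it.
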(event `self.ReceiveBeginPlay`
  (bind _lifetimerange (`self.LifetimeRange`))
  (bind _impulsestrengthrange (`self.ImpulseStrengthRange`))
  (set `self.CurrentLifetimeBeforeKill` (`KismetMathLibrary.RandomFloatInRange` (`.Value` (break `FloatRangeBound` (break `FloatRange` _lifetimerange))) (`.Value` (break `FloatRangeBound` (`.UpperBound` (break `FloatRange` _lifetimerange))))))
  (bind _output_get (set `self.StartingScale` (`KismetArrayLibrary.Array_Random` (`self.PossibleStartingScales`))))
  (`self.SetActorScale3D` _output_get)
  (`PrimitiveComponent.AddImpulse` (`self.StaticMeshComponent`) (* (`self.ImpulseDirection`) (`KismetMathLibrary.RandomFloatInRange` (`.Value` (break `FloatRangeBound` (break `FloatRange` _impulsestrengthrange))) (`.Value` (break `FloatRangeBound` (`.UpperBound` (break `FloatRange` _impulsestrengthrange)))))) "None" false))

(event `self.ReceiveTick`
  (params (DeltaSeconds :type "Float (single-precision)"))
  (bind _return (`/Game/o_Libraries/BPL_GeneralUtilities.Decrease Value Float` (`self.CurrentLifetimeBeforeKill`) DeltaSeconds))
  ;[1 1 1 0.33] if in the last second, get smaller before destroying
  (if (<= _return 1.0)
    (`self.SetActorScale3D` (* (`self.StartingScale`) (`self.CurrentLifetimeBeforeKill`)))
    (if (<= (`self.CurrentLifetimeBeforeKill`) 0.0)
      (`self.K2_DestroyActor`))))

(fn `UserConstructionScript`)