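; BP_Clock is a clock actor that animates its hand components by rotating them on Tick.
; Second and SecondReverse step by a fixed local pitch every frame, so their speed depends on frame rate rather than real time.
; MinutesTimer counts frames and, after each full turn of Second, resets and steps Minute, along with an extra step for SecondReverse.
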(event `self.ReceiveTick`
  (params (DeltaSeconds :type "Float (single-precision)"))
  (`SceneComponent.K2_AddLocalRotation` (`self.Second`) (`KismetMathLibrary.MakeRotator` 0.0 -10.0) false false)
  (`SceneComponent.K2_AddLocalRotation` (`self.Second Reverse`) (`KismetMathLibrary.MakeRotator` 0.0 -10.0) false false)
  (bind _result (`/Engine/EditorBlueprintResources/StandardMacros.IncrementFloat` (`self.Minutes Timer`))
    (:`  `
      (if (== _result 36.0)
        (set `self.Minutes Timer` 0.0)
        (`SceneComponent.K2_AddLocalRotation` (`self.Minute`) (`KismetMathLibrary.MakeRotator` 0.0 -10.0) false false)
        (`SceneComponent.K2_AddLocalRotation` (`self.Second Reverse`) (`KismetMathLibrary.MakeRotator` 0.0 -10.0) false false)))))

(fn `UserConstructionScript`)