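; Toggleable cheat function that shows an on-screen controller input visualizer for the Metro player controller.
; Toggling on lazily creates the widget, registers it on the controller and adds its Enhanced Input mapping context; toggling off removes both widget and context.
; A next-tick retry loop waits for the input subsystem to become valid.
; Gamepad-detection auto-activation is unwired because the device query returns false positives.
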(event `self.OnInit`
  (bind _cheatmanager (`self.CheatManager`)
    (:`then`
      (bind _asbp_metro_player_controller (cast `/Game/Design/_GameManagement/Core/BP_MetroPlayerController` (`CheatManager.GetPlayerController` _cheatmanager)))
      (set `self.PlayerController` _asbp_metro_player_controller))
    (:`else`)))

(event `self.OnCheat`
  (bind _returnvalue (pcsubsystem `EnhancedInputLocalPlayerSubsystem` (`self.PlayerController`)))
  (if (`self.bIsToggled`)
    (`self.VisualizerWidget`
      (:`then`
        _)
      (:`else`
        (`self.CreateWidget`)))
    (`UserWidget.AddToViewport` (`self.VisualizerWidget`) 0)
    ;[1 1 1 0.33] I know the "Delay until valid" is HORRIBLE, but on BeginPlay the Subsystem isn't valid...
    ; Sorry!!!
    (`/Engine/EditorBlueprintResources/StandardMacros.IsValid` _returnvalue :!label _label
      (:`Is Valid`
        (`EnhancedInputSubsystemInterface.AddMappingContext` _returnvalue "/Game/Design/_GameManagement/Input/Visualizer/IMC_ControllerVisualizer.IMC_ControllerVisualizer" 10 (make `ModifyContextOptions` false)))
      (:`Is Not Valid`
        (`KismetSystemLibrary.DelayUntilNextTick`)
        (goto _label)))
    (else
      (`Widget.RemoveFromParent` (`self.VisualizerWidget`))
      (`EnhancedInputSubsystemInterface.RemoveMappingContext` (pcsubsystem `EnhancedInputLocalPlayerSubsystem` (`self.PlayerController`)) "/Game/Design/_GameManagement/Input/Visualizer/IMC_ControllerVisualizer.IMC_ControllerVisualizer" (make `ModifyContextOptions` false)))))

(fn `CreateWidget`
  (bind _returnvalue (`|CreateWidget` "/Game/Design/Widgets/InputVisualizers/WBP_ControllerInputsVisualizer.WBP_ControllerInputsVisualizer_C"))
  (bind _output_get (set `self.VisualizerWidget` _returnvalue))
  (set `/Game/Design/_GameManagement/Core/BP_MetroPlayerController.ControllerInputVisualizer` _output_get (`self.PlayerController`)))