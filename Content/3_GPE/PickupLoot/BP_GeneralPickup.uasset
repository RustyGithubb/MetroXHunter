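; BP_GeneralPickup is a pickup actor that transfers a typed amount of loot into an inventory when interacted with.
; Its sphere trigger caches the BP_InventoryComponent of any overlapping actor that has one.
; On Interact, it calls AddToInventory with its type and amount, stores the returned value as the remaining amount, and destroys itself when that reaches zero.
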(event `self.Interact`
  (bind _playerinventory (`self.PlayerInventory`)
    (:`then`
      (bind _overflow (`/Game/0_Design/GameManagement_/BP_InventoryComponent.AddToInventory` _playerinventory (`self.PickupType`) (`self.Amount`)))
      (bind _output_get (set `self.Amount` _overflow))
      (if (== _output_get 0)
        (`self.K2_DestroyActor`)))
    (:`else`)))

(event `self.SphereTrigger.OnComponentBeginOverlap`
  (params (OverlappedComponent :type "PrimitiveComponent Object Reference") (OtherActor :type "Actor Object Reference") (OtherComp :type "PrimitiveComponent Object Reference") (OtherBodyIndex :type Integer) (bFromSweep :type Boolean) (SweepResult :type "HitResult Structure (by ref)"))
  (bind _returnvalue (`self.GetComponentByClass` OtherActor "/Game/0_Design/GameManagement_/BP_InventoryComponent.BP_InventoryComponent_C"))
  (`/Engine/EditorBlueprintResources/StandardMacros.IsValid` _returnvalue
    (:`Is Valid`
      (set `self.PlayerInventory` _returnvalue))))

(fn `UserConstructionScript`)