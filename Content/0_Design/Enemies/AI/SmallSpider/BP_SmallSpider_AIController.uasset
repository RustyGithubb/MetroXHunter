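; AI controller for the small spider enemy that runs its behavior tree and writes state, target and radii to the Blackboard.
; Spider shriek and death events drive state changes, and received shrieks can make it chase the player.
; It reserves tokens on the target's AITargetComponent, whose group placement sets the reposition radius.
; An overridden or random personality scales the mesh; its near-death frenzy/flee reaction is currently disconnected.
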(event `self.ReceiveBeginPlay`)

(event `self.ReceiveTick`
  (params (DeltaSeconds :type "Float (single-precision)"))
  (`self.TickDebugDraw`))

(event `self.ReceivePossess`
  (params (PossessedPawn :type "Pawn Object Reference"))
  (`KismetSystemLibrary.DelayUntilNextTick`)
  (`self.RetrieveReferences`)
  (`self.InitPersonality`)
  (`self.RunBehaviorTree` "/Game/0_Design/Enemies/AI/SmallSpider/BT_SmallSpider.BT_SmallSpider")
  (`self.SetActorTickEnabled` true)
  (if (`/Game/0_Design/Enemies/AI/SmallSpider/BP_SmallSpider.bChasePlayerOnBeginPlay` (`self.Spider`))
    (`self.ChasePlayer` true)))

(event `self.ReceiveUnPossess`
  (params (UnpossessedPawn :type "Pawn Object Reference"))
  (`self.SetActorTickEnabled` false))

(event `OnShriekStateChanged`
  (params (Spider :type "/Game/0_Design/Enemies/AI/SmallSpider/BP_SmallSpider Object Reference") (IsStarted :type Boolean))
  (`self.SetState` (select `bool` IsStarted :`false` (select `bool` (`/Game/0_Design/Enemies/AI/SmallSpider/BP_SmallSpider.bIsDead` Spider) :`false` "NewEnumerator1" :`true` "NewEnumerator3" :!type "/Game/0_Design/Enemies/AI/SmallSpider/Enums/E_SmallSpider_AIState Enum") :`true` "NewEnumerator4")))

(event `OnShriekReceive`
  (params (EmissionContext :type "/Game/0_Design/Enemies/Shriek/F_ShriekEmissionContext Structure"))
  (if (not (`/Game/0_Design/Enemies/AI/SmallSpider/BP_SmallSpider.bIsDead` (`self.Spider`)))
    (`self.ChasePlayer` (select `/Game/0_Design/Enemies/AI/SmallSpider/Enums/E_SmallSpider_AIState` (`self.GetState`) :`NewEnumerator0` true :`NewEnumerator1` true))))

(event `OnDeath`
  (`self.SetState` "NewEnumerator3")
  (bind _currentaitarget (`self.CurrentAITarget`)
    (:`then`
      (`/Game/0_Design/Enemies/AI/BP_AITargetComponent.FreeReservations` _currentaitarget self))
    (:`else`)))

(event `/Game/0_Design/Enemies/AI/BPI_AITarget_GroupPlaceReserver.OnGroupPlaceUpdated`
  (params (AITarget :type "/Game/0_Design/Enemies/AI/BP_AITargetComponent Object Reference") (GroupIndex :type Integer))
  (bind (_lowerbound _upperbound) (break `FloatRange` (`|GetArrayItem` (`/Game/0_Design/Enemies/AI/BP_AITargetComponent.GroupDistances` AITarget) GroupIndex)))
  (`self.Set Group Place Index` GroupIndex)
  (set `self.GroupRepositionRadius` (`KismetMathLibrary.RandomFloatInRange` (`.Value` (break `FloatRangeBound` _lowerbound)) (`.Value` (break `FloatRangeBound` _upperbound))))
  (`self.UpdateRepositionRadius`))

(fn `ChasePlayer`
  (params (ShouldChangeState :type Boolean :default true))
  (bind _returnvalue (`GameplayStatics.GetGameMode`))
  (bind _returnvalue_2 (`GameModeBase.K2_FindPlayerStart` _returnvalue null "Start"))
  ;[1 1 1 0.33] Target MainChara
  (bind _returnvalue_3 (`KismetSystemLibrary.LoadClassAsset_Blocking` (`self.PlayerClass`)))
  (bind _asactor (castclass `Actor` _returnvalue_3)
    (:`then`
      (bind _returnvalue_4 (`GameplayStatics.GetActorOfClass` _asactor)) ; Use this function instead of GetPlayerPawn so while in debug camera, \nthey still target the main character
      (`/Engine/EditorBlueprintResources/StandardMacros.IsValid` _returnvalue_4
        (:`Is Valid`
          (`self.ChaseTarget` _returnvalue_4 ShouldChangeState))
        (:`Is Not Valid`
          (`/Engine/EditorBlueprintResources/StandardMacros.IsValid` _returnvalue_2 :!label _label
            (:`Is Valid`
              (`self.ChaseTarget` _returnvalue_2 ShouldChangeState))
            (:`Is Not Valid`
              (`self.ChaseTarget` (`GameModeBase.K2_FindPlayerStart` _returnvalue null "None") ShouldChangeState))))))
    (:`CastFailed`
      (goto _label))))

(fn `ChaseTarget`
  (params (Target :type "Actor Object Reference") (ShouldChangeState :type Boolean :default true))
  (`BlackboardComponent.SetValueAsObject` (`self.Blackboard`) "TargetActor" Target)
  (bind _output_get (set `self.CurrentAITarget` (`self.GetComponentByClass` Target "/Game/0_Design/Enemies/AI/BP_AITargetComponent.BP_AITargetComponent_C"))) ; Get AITargetComponent
  (`/Engine/EditorBlueprintResources/StandardMacros.IsValid` _output_get
    (:`Is Valid`
      _)
    (:`Is Not Valid`
      (`KismetSystemLibrary.PrintText` (`|FormatText` "SmallSpiderAI: Can't find AITargetComponent on {Actor}! Please provide one!" Target) true true (struct :`R` 1.0 :`A` 1.0) 5.0 "SmallSpiderAI_NoAITargetComponent")))
  (`BlackboardComponent.SetValueAsObject` (`self.Blackboard`) "AITargetComponent" _output_get)
  (if ShouldChangeState
    (`self.SetState` "NewEnumerator1")))

(fn `ClimbTo`
  (params (Destination :type "Vector Structure"))
  (`BlackboardComponent.SetValueAsVector` (`self.Blackboard`) "MoveLocation" Destination)
  (`self.SetState` "NewEnumerator2")
  (`self.StopMovement`))

(fn `FreeTargetToken`
  (params (Target :type "/Game/0_Design/Enemies/AI/BP_AITargetComponent Object Reference") (Tokens :type Integer))
  (`/Game/0_Design/Enemies/AI/BP_AITargetComponent.FreeTokens` Target self Tokens))

(fn `GetChasedTarget`
  (returns (Target :type "Actor Object Reference"))
  (return (cast `Actor` (`BlackboardComponent.GetValueAsObject` (`self.Blackboard`) "TargetActor") :!pure true)))

(fn `GetEQSContextActor`
  (returns (Actor :type "Actor Object Reference"))
  (return (select `bool` (`self.bIsRunningAway`) :`false` (`self.GetChasedTarget`) :`true` (`self.RunAwayActor`))))

(fn `GetState`
  (returns (State :type "/Game/0_Design/Enemies/AI/SmallSpider/Enums/E_SmallSpider_AIState Enum"))
  (return (cast `/Game/0_Design/Enemies/AI/SmallSpider/Enums/E_SmallSpider_AIState` (`BlackboardComponent.GetValueAsEnum` (`self.Blackboard`) "State"))))

(fn `InitPersonality`
  (bind _mesh (`Character.Mesh` (`self.Spider`)))
  ;[1 1 1 0.33] Apply overriden personality
  (bind _returnvalue (`KismetSystemLibrary.LoadAsset_Blocking` (`/Game/0_Design/Enemies/AI/SmallSpider/BP_SmallSpider.OverridenPersonality` (`self.Spider`)))) ; It's probably already loaded by the array, right?
  (bind _asbp_spider_personality_data (cast `/Game/0_Design/Enemies/AI/SmallSpider/BP_SpiderPersonalityData` _returnvalue)
    (:`then`
      (set `self.PersonalityData` _asbp_spider_personality_data))
    (:`CastFailed`
      ;[1 1 1 0.33] Randomize personality
      (set `self.PersonalityData` (`KismetArrayLibrary.Array_Random` (`self.PersonalitiesDatas`)))))
  ;[1 1 1 0.33] Scale depending on personality
  (`SceneComponent.SetWorldScale3D` _mesh (* (`SceneComponent.K2_GetComponentScale` _mesh) (`/Game/0_Design/Enemies/AI/SmallSpider/BP_SpiderPersonalityData.MeshOffsetScale` (`self.PersonalityData`)))))

(fn `ReactToNearDeath`
  (params (DeadSpider :type "Actor Object Reference")))

(fn `ReceiveEvent`
  (params (CalledTag :type "GameplayTag Structure") (CallingObject :type "Object Object Reference (by ref)"))
  (returns (Return :type Boolean))
  (if (not (`/Game/0_Design/Enemies/AI/SmallSpider/BP_SmallSpider.bIsDead` (`self.Spider`)))
    (if (!= CallingObject (`self.Spider`))
      (`|SwitchGameplayTag` CalledTag
        (:`Default`
          (return false))
        (:`Event.SmallSpider.Death`
          (`self.ReactToNearDeath` (cast `Actor` CallingObject :!pure true)))))))

(fn `ReserveTargetToken`
  (params (Target :type "/Game/0_Design/Enemies/AI/BP_AITargetComponent Object Reference") (Tokens :type Integer))
  (returns (bIsSuccess :type Boolean))
  (bind _bissuccess (`/Game/0_Design/Enemies/AI/BP_AITargetComponent.ReserveTokens` Target self Tokens))
  (set `self.CurrentAITarget` Target)
  (return _bissuccess))

(fn `RetrieveReferences`
  (bind _asbp_small_spider (cast `/Game/0_Design/Enemies/AI/SmallSpider/BP_SmallSpider` (`self.K2_GetPawn`))
    (:`then`
      (bind _output_get (set `self.Spider` _asbp_small_spider))
      (add `/Game/0_Design/Enemies/AI/SmallSpider/BP_SmallSpider.OnDeath` _output_get (`|CreateDelegate` :!event `OnDeath`))
      (add `/Game/0_Design/Enemies/AI/SmallSpider/BP_SmallSpider.OnShriekStateChanged` _output_get (`|CreateDelegate` :!event `OnShriekStateChanged`))
      (add `/Game/0_Design/Enemies/Shriek/BP_ShriekReceiverComponent.OnShriekReceived` (`/Game/0_Design/Enemies/AI/SmallSpider/BP_SmallSpider.BP_ShriekReceiverComponent` _output_get) (`|CreateDelegate` :!event `OnShriekReceive`))
      (`/EventDispatcherHub/FunctionLibrary/BPL_EventDispatcherHub.Bind to Single Gameplay Event` (struct :`TagName` "Event.SmallSpider.Death") self))
    (:`CastFailed`
      (`KismetSystemLibrary.PrintText` "SmallSpider_AIController: Can't cast controlled pawn to BP_SmallSpider!" true true (struct :`R` 1.0 :`A` 1.0) 5.0))))

(fn `Set Group Place Index`
  (params (GroupIndex :type Integer))
  (bind _output_get (set `self.TargetGroupPlaceIndex` GroupIndex))
  (`BlackboardComponent.SetValueAsInt` (`self.Blackboard`) "GroupPlaceIndex" _output_get))

(fn `SetRepositionRadius`
  (params (Radius :type "Float (double-precision)"))
  (`BlackboardComponent.SetValueAsFloat` (`self.Blackboard`) "RepositionRadius" Radius))

(fn `SetRunAwayRadius`
  (params (Radius :type "Float (double-precision)"))
  (`BlackboardComponent.SetValueAsFloat` (`self.Blackboard`) "RunAwayRadius" Radius))

(fn `SetState`
  (params (State :type "/Game/0_Design/Enemies/AI/SmallSpider/Enums/E_SmallSpider_AIState Enum" :default "NewEnumerator0"))
  (`BlackboardComponent.SetValueAsEnum` (`self.Blackboard`) "State" State))

(fn `TickDebugDraw`
  (bind _blackboard (`self.Blackboard`))
  (bind _spider (`self.Spider`))
  (bind _returnvalue (`self.K2_GetActorLocation` (`self.K2_GetPawn`)))
  (if (`MXHUtilityLibrary.IsCVarAIDebugEnabled`)
    ;[0.2667 0 1 0.33] Draw Blackboard State
    (`KismetSystemLibrary.DrawDebugString` _returnvalue (`KismetTextLibrary.Conv_TextToString` (`|FormatText` "Self: {Name} \nState: {State} \nTarget: {Target} \nAttackJumpCooldown: {AttackJumpCooldown}s \nShriekTime: {ShriekTime}s \nShriekLife: {ShriekLife} HP \nGroupPlaceIndex: {GroupPlaceIndex} \nbIsFrenzy: {bIsFrenzy} \nPersonality: {Personality}" self (`|GetEnumeratorNameAsString` (cast `/Game/0_Design/Enemies/AI/SmallSpider/Enums/E_SmallSpider_AIState` (`BlackboardComponent.GetValueAsEnum` _blackboard "State"))) (`KismetSystemLibrary.GetDisplayName` (`BlackboardComponent.GetValueAsObject` _blackboard "TargetActor")) (`KismetMathLibrary.FMax` (`/Game/0_Design/Enemies/AI/SmallSpider/BP_SmallSpider.CurrentAttackJumpCooldown` _spider)) (`KismetSystemLibrary.K2_GetTimerRemainingTimeHandle` (`/Game/0_Design/Enemies/AI/SmallSpider/BP_SmallSpider.ShriekTimer` _spider)) (`/Game/0_Design/LifeSystem/BP_LifeComponent.CurrentLife` (`/Game/0_Design/Enemies/AI/SmallSpider/BP_SmallSpider.BP_LifeComponent_Shriek` _spider)) (`self.TargetGroupPlaceIndex`) (`self.bIsFrenzy`) (`/Game/0_Design/Enemies/AI/SmallSpider/BP_SpiderPersonalityData.Name` (`self.PersonalityData`)))) null (`KismetMathLibrary.SelectColor` (struct :`R` 0.566536 :`G` 0.556641 :`B` 0.59375 :`A` 1.0) (struct :`R` 0.969444 :`G` 0.958333 :`B` 1.0 :`A` 1.0) (`/Game/0_Design/Enemies/AI/SmallSpider/BP_SmallSpider.bIsDead` (`self.Spider`))))
    ;[0 0.8333 1 0.33] Draw Control Rotation
    (`KismetSystemLibrary.DrawDebugArrow` _returnvalue (+ _returnvalue (* (`KismetMathLibrary.GetForwardVector` (`self.GetControlRotation`)) 150.0)) 2.0 (struct :`G` 0.833333 :`B` 1.0 :`A` 1.0) 0.0 4.0)))

(fn `UpdateRepositionRadius`
  (`self.SetRepositionRadius` (+ (`self.GroupRepositionRadius`) (`self.PersonalityRepositionRadius`))))

(fn `UserConstructionScript`)