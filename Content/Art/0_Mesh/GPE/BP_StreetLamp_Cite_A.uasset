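; Three-bulb street lamp whose bulbs shatter individually when damaged and which exposes its lights to a flicker system.
; TakeDamage reads the hit component's first tag as a bulb index, destroys that bulb and light, and plays its Vertex Animation Texture via timeline.
; A counter seeded from LightsON drops per break, removing ambient light and audio at zero.
; Flicker callbacks swap and restore bulb materials, though Bulb2's swap is disconnected.
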(event `self.ReceiveBeginPlay`
  (`KismetArrayLibrary.Array_Add` (`self.Materials`) (`PrimitiveComponent.GetMaterial` (`self.Bulb_0`) 0))
  (`KismetArrayLibrary.Array_Add` (`self.Materials`) (`PrimitiveComponent.GetMaterial` (`self.Bulb_1`) 0))
  (`KismetArrayLibrary.Array_Add` (`self.Materials`) (`PrimitiveComponent.GetMaterial` (`self.Bulb_2`) 0))
  (set `self.AmbiantLightIntensity` (`LightComponentBase.Intensity` (`self.AmbiantLight`)))
  (for _array_element (`self.LightsON`)
    (if _array_element
      (`/Engine/EditorBlueprintResources/StandardMacros.IncrementInt` (`self.LightBulbLeft`)))))

(event `OnBulbDestroyed`
  (bind _result (`/Engine/EditorBlueprintResources/StandardMacros.DecrementInt` (`self.LightBulbLeft`))
    (:`  `
      (if (== _result 0)
        (`ActorComponent.K2_DestroyComponent` (`self.AmbiantLight`))
        (`AudioComponent.Stop` (`self.Audio`))))))

(event `PLAY VAT`
  (params (TargetVAT :type Integer))
  ;[1 1 1 0.33] NEED REFACTOR
  (`self.OnBulbDestroyed`)
  (switch `int` TargetVAT
    (:`0`
      (`ActorComponent.K2_DestroyComponent` (`self.Bulb_0`))
      (`ActorComponent.K2_DestroyComponent` (`self.Light_Bulb0`))
      (`SceneComponent.SetHiddenInGame` (`self.VAT_Bulb_0`) false false)
      (bind (_direction _animation) (`Timeline|Timeline` :!via `PlayFromStart`)
        (:`Update`
          (`MeshComponent.SetScalarParameterValueOnMaterials` (`self.VAT_Bulb_0`) "Display Frame" (+ (* _animation 239.0) 1.0)))))
    (:`1`
      (`ActorComponent.K2_DestroyComponent` (`self.Bulb_1`))
      (`ActorComponent.K2_DestroyComponent` (`self.Light_Bulb1`))
      (`SceneComponent.SetHiddenInGame` (`self.VAT_Bulb_1`) false false)
      (bind (_direction_2 _animation_2) (`Timeline|Timeline_0` :!via `PlayFromStart`)
        (:`Update`
          (`MeshComponent.SetScalarParameterValueOnMaterials` (`self.VAT_Bulb_1`) "Display Frame" (+ (* _animation_2 239.0) 1.0)))))
    (:`2`
      (`ActorComponent.K2_DestroyComponent` (`self.Bulb_2`))
      (`ActorComponent.K2_DestroyComponent` (`self.Light_Bulb2`))
      (`SceneComponent.SetHiddenInGame` (`self.VAT_Bulb_2`) false false)
      (bind (_direction_3 _animation_3) (`Timeline|Timeline_1` :!via `PlayFromStart`)
        (:`Update`
          (`MeshComponent.SetScalarParameterValueOnMaterials` (`self.VAT_Bulb_2`) "Display Frame" (+ (* _animation_3 239.0) 1.0)))))))

(fn `CanCallTakeDamage`
  (params (DamageContext :type "DamageContext Structure (by ref)"))
  (returns (ReturnValue :type Boolean))
  (return true))

(fn `IsShownAsDamageableToPlayer`
  (params (DamageType :type "EDamageType Enum" :default "Generic"))
  (returns (ReturnValue :type Boolean))
  (return false))

(fn `OnFlickLightStart`
  (params (LightData :type "LightData Structure (by ref)"))
  (`|ExecutionSequence`
    (:`then_0`
      (if (`|GetArrayItem` (`self.LightsON`))
        (bind _bulb_0 (`self.Bulb_0`)
          (:`then`
            (`PrimitiveComponent.SetMaterial` _bulb_0 0 "/Game/Design/GPE/Destructible/Lights/MI_BulbTEST.MI_BulbTEST"))
          (:`else`))))
    (:`then_1`
      (if (`|GetArrayItem` (`self.LightsON`) 1)
        (bind _bulb_1 (`self.Bulb_1`)
          (:`then`
            (`PrimitiveComponent.SetMaterial` _bulb_1 0 "/Game/Design/GPE/Destructible/Lights/MI_BulbTEST.MI_BulbTEST"))
          (:`else`))))
    (:`then_2`
      (if (`|GetArrayItem` (`self.LightsON`) 2)
        (bind _bulb_2 (`self.Bulb_2`)
          (:`then`)
          (:`else`))))
    (:`then_3`
      (setmembers `LightData` :`StructRef` LightData :`OriginalLightIntensity` (`self.AmbiantLightIntensity`)))))

(fn `OnFlickLightStop`
  (params (LightData :type "LightData Structure (by ref)"))
  (`|ExecutionSequence`
    (:`then_0`
      (bind _bulb_0 (`self.Bulb_0`)
        (:`then`
          (`PrimitiveComponent.SetMaterial` _bulb_0 0 (`|GetArrayItem` (`self.Materials`))))
        (:`else`)))
    (:`then_1`
      (bind _bulb_1 (`self.Bulb_1`)
        (:`then`
          (`PrimitiveComponent.SetMaterial` _bulb_1 0 (`|GetArrayItem` (`self.Materials`) 1)))
        (:`else`)))
    (:`then_2`
      (bind _bulb_2 (`self.Bulb_2`)
        (:`then`
          (`PrimitiveComponent.SetMaterial` _bulb_2 0 (`|GetArrayItem` (`self.Materials`) 2)))
        (:`else`)))
    (:`then_3`
      (`|ExecutionSequence`
        (:`then_0`
          (bind _light_bulb0 (`self.Light_Bulb0`)
            (:`then`
              (`LightComponent.SetIntensity` _light_bulb0 0.0))
            (:`else`)))
        (:`then_1`
          (bind _light_bulb2 (`self.Light_Bulb2`)
            (:`then`
              (`LightComponent.SetIntensity` _light_bulb2 0.0))
            (:`else`)))
        (:`then_2`
          (bind _light_bulb1 (`self.Light_Bulb1`)
            (:`then`
              (`LightComponent.SetIntensity` _light_bulb1 0.0))
            (:`else`)))
        (:`then_3`
          (return))))))

(fn `OnFlickLightTick`
  (params (DeltaTime :type "Float (single-precision)") (LightData :type "LightData Structure (by ref)"))
  (return))

(fn `OnFlickLightUpdate`
  (params (LightData :type "LightData Structure (by ref)") (IntensityScale :type "Float (single-precision)"))
  (return))

(fn `RetrieveFlickableLights`
  (returns (ReturnValue :type "Array of LightComponent Object Reference"))
  (locals (FlickableLights :type "Array of LightComponent Object Reference"))
  (bind _flickablelights (`local.FlickableLights`))
  (`|ExecutionSequence`
    (:`then_0`
      (if (`|GetArrayItem` (`self.LightsON`))
        (`KismetArrayLibrary.Array_Add` (`local.FlickableLights`) (`self.Light_Bulb0`))))
    (:`then_1`
      (if (`|GetArrayItem` (`self.LightsON`) 1)
        (`KismetArrayLibrary.Array_Add` (`local.FlickableLights`) (`self.Light_Bulb1`))))
    (:`then_2`
      (if (`|GetArrayItem` (`self.LightsON`) 2)
        (`KismetArrayLibrary.Array_Add` (`local.FlickableLights`) (`self.Light_Bulb2`))))
    (:`then_3`
      (`KismetArrayLibrary.Array_Add` _flickablelights (`self.AmbiantLight`))
      (return _flickablelights))))

(fn `TakeDamage`
  (params (DamageContext :type "DamageContext Structure (by ref)"))
  (returns (ReturnValue :type Boolean))
  (bind (_bblockinghit _binitialoverlap _time _distance _location _impactpoint _normal _impactnormal _physmat _hitactor _hitcomponent) (`GameplayStatics.BreakHitResult` (`.HitResult` (break `DamageContext` DamageContext))))
  (bind _componenttags (`ActorComponent.ComponentTags` _hitcomponent))
  (`/Engine/EditorBlueprintResources/StandardMacros.IsValid` _hitcomponent
    (:`Is Valid`
      (if (`KismetArrayLibrary.Array_IsNotEmpty` _componenttags)
        (`self.PLAY VAT` (`KismetStringLibrary.Conv_StringToInt` (`KismetStringLibrary.Conv_NameToString` (`|GetArrayItem` _componenttags))))))
    (:`Is Not Valid`
      _))
  (return false))

(fn `UserConstructionScript`)