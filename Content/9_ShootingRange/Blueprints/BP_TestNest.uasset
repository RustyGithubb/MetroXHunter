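; BP_TestNest is a spider spawner in the shooting range that spawns one BP_Spider at its own transform on BeginPlay.
; A starting NbOfSpider of zero enables infinite spawning; otherwise the count limits spawns.
; When NoGravity is set, it zeroes the spider's gravity, decrements the count and binds OnDeath to respawn.
; That countdown and respawn chain runs only on the NoGravity branch.
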(event `self.ReceiveBeginPlay`
  ;[1 1 1 0.33] Check if User want infinite spawn
  (if (== (`self.NbOfSpider`) 0)
    (set `self.InfiniteSpawn` true))
  (`self.SpawnMonster`))

(event `SpawnMonster`
  ;[1 1 1 0.33] NbOrInfiniteSpawn condition check
  (if (or (> (`self.NbOfSpider`) 0) (`self.InfiniteSpawn`))
    (bind _returnvalue (`|SpawnActorFromClass` "/Game/9_ShootingRange/Blueprints/BP_Spider.BP_Spider_C" (`self.GetTransform`) "Undefined" "MultiplyWithRoot" null null))
    ;[1 1 1 0.33] Check if user don't want gravity
    (if (`self.No Gravity`)
      (set `CharacterMovementComponent.GravityScale` 0.0 (`Character.CharacterMovement` _returnvalue))
      ;[1 1 1 0.33] Reduce Nb of Spider
      (bind _result (`/Engine/EditorBlueprintResources/StandardMacros.DecrementInt` (`self.NbOfSpider`))
        (:`  `
          (set `self.NbOfSpider` _result)
          (add `/Game/9_ShootingRange/Blueprints/BP_Spider.OnDeath` _returnvalue (delegate `SpawnMonster`)))))))

(fn `UserConstructionScript`)