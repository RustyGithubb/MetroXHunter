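; BP_StreetLamp_Cite_B is a street lamp with a SpotLight and a bulb mesh that responds to light flicker callbacks.
; It caches Bulb1's original material on BeginPlay, swaps in MI_BulbTEST when a flicker starts and restores the original when it stops.
; It exposes the SpotLight as its only flickable light, leaving the flicker tick and update callbacks empty.
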(event `self.ReceiveBeginPlay`
  (`KismetArrayLibrary.Array_Add` (`self.Materials`) (`PrimitiveComponent.GetMaterial` (`self.Bulb_1`) 0)))

(fn `OnFlickLightStart`
  (params (LightData :type "LightData Structure (by ref)"))
  (`PrimitiveComponent.SetMaterial` (`self.Bulb_1`) 0 "/Game/Design/GPE/Destructible/Lights/MI_BulbTEST.MI_BulbTEST"))

(fn `OnFlickLightStop`
  (params (LightData :type "LightData Structure (by ref)"))
  (`PrimitiveComponent.SetMaterial` (`self.Bulb_1`) 0 (`|GetArrayItem` (`self.Materials`)))
  (return))

(fn `OnFlickLightTick`
  (params (DeltaTime :type "Float (single-precision)") (LightData :type "LightData Structure (by ref)"))
  (return))

(fn `OnFlickLightUpdate`
  (params (LightData :type "LightData Structure (by ref)") (IntensityScale :type "Float (single-precision)"))
  (return))

(fn `RetrieveFlickableLights`
  (returns (ReturnValue :type "Array of LightComponent Object Reference"))
  (return (`|MakeArray` (`self.SpotLight`) :!type "LightComponent Object Reference")))

(fn `UserConstructionScript`)