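; Settings unit that controls the overall renderer quality in the game's display graphics options.
; On initialize it fills the RendererQuality array with the five scalability levels.
; On apply it sets the overall scalability level from the selected index through GameUserSettings and applies non-resolution settings.
; An index of -1 means custom settings, so it prints a notice and applies settings without changing the overall level.
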(event `self.OnApplySetting`
  (params (bInGame :type Boolean))
  (if (!= (`self.IndexValue`) -1)
    (bind _returnvalue (`GameUserSettings.GetGameUserSettings`))
    (`GameUserSettings.SetOverallScalabilityLevel` _returnvalue (`|GetArrayItem` (`self.RendererQuality`) (`self.IndexValue`)))
    (`GameUserSettings.ApplyNonResolutionSettings` _returnvalue)
    (else
      (`KismetSystemLibrary.PrintString` "CUSTOM SETTINGS")
      (bind _returnvalue_2 (`GameUserSettings.GetGameUserSettings`))
      (`GameUserSettings.ApplyNonResolutionSettings` _returnvalue_2))))

(event `self.OnInitialize`
  (for _index (range 5)
    (`KismetArrayLibrary.Array_Add` (`self.RendererQuality`) _index)))