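; Cheat function that loads a map chosen from a configured list of levels.
; On init it copies each level's display name into the selectable value names.
; Triggering the cheat on a different index than last time only records that index.
; Triggering it again on the same index opens that level by soft reference with absolute travel, provided the reference is valid.
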(event `self.OnInit`
  (for _array_element (`self.Levels`)
    (`KismetArrayLibrary.Array_Add` (`self.ValueNames`) (break `GameLevelReference` _array_element))))

(event `self.OnCheat`
  (bind _index (`self.Index`))
  (bind (_displayname _level) (break `GameLevelReference` (`|GetArrayItem` (`self.Levels`) _index)))
  (if (== (`self.LastIndex`) _index)
    (if (`KismetSystemLibrary.IsValidSoftObjectReference` _level)
      (`GameplayStatics.OpenLevelBySoftObjectPtr` _level))
    (else
      (set `self.LastIndex` _index))))