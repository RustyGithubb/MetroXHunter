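; Openable locker interactable that swings its door open and spawns a pickup inside.
; Interacting locks it and messages the player character; an Event.Locker.Open gameplay event then opens it, although BeginPlay binds to Event.Locker.PressCorrect.
; Opening async-loads the item class, spawns it with the set amount, then plays the door timeline.
; Interaction colliders are disabled before destruction so overlapping components release the locker safely, preventing null references and blocked interactions.
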(event `self.ReceiveBeginPlay`
  (`parent.ReceiveBeginPlay`)
  (set `self.PlayerCharacter` (`GameplayStatics.GetPlayerPawn` 0))
  (`/EventDispatcherHub/FunctionLibrary/BPL_EventDispatcherHub.Bind to Multiple Gameplay Events` (struct :`GameplayTags` (struct :`(TagName` "Event.Locker.PressCorrect") :`(TagName` "Event.Locker.PressWrong") :`(TagName` "Event.Locker.Open"))) self)
  (`SceneComponent.K2_SetRelativeRotation` (`self.Door`) (`KismetMathLibrary.MakeRotator` 0.0 0.0 -180.0) false false))

(event `self.InteractableComponent.OnInteract`
  (if (`self.HasBeenOpen`)
    _
    (elif (not (`self.isLockedInInteraction`))
      (message `/Game/0_Design/GameManagement_/BPI_MainPlayerCharacter.InteractWithLocker` (`self.PlayerCharacter`) self)
      (set `self.isLockedInInteraction` true))))

(event `OpenDoor`
  (bind _class (`|LoadAssetClass` (`self.ItemInsideLocker`))
    (:`Completed`
      (bind _asbp_general_pickup (castclass `/Game/3_GPE/PickupLoot/BP_GeneralPickup` _class))
      (bind _returnvalue (`|SpawnActorFromClass` _asbp_general_pickup (`KismetMathLibrary.MakeTransform` (`SceneComponent.K2_GetComponentLocation` (`self.ItemSpawnPoint`))) "Undefined" "MultiplyWithRoot" null null))
      (set `/Game/3_GPE/PickupLoot/BP_GeneralPickup.Amount` (`self.ItemAmount`) _returnvalue)
      (set `self.HasBeenOpen` true)
      ;[1 1 1] Prevent the PlayerCharacter from thinking that this can be interacted (and blocking other interactables)
      ; Also removing colliders for better performance.
      ;
      ; To avoid any errors, we set collisions to NoCollision first so that the components register "we lost the Interactable Object" before destroying it, to avoid any NullReferenceException
      (`PrimitiveComponent.SetCollisionEnabled` (`self.InnerInteraction`) "NoCollision")
      (`PrimitiveComponent.SetCollisionEnabled` (`self.OutterInteraction`) "NoCollision")
      (`ActorComponent.K2_DestroyComponent` (`self.Widget`))
      (`ActorComponent.K2_DestroyComponent` (`self.InteractableComponent`))
      (`ActorComponent.K2_DestroyComponent` (`self.InnerInteraction`))
      (`ActorComponent.K2_DestroyComponent` (`self.OutterInteraction`))
      (bind (_direction _doorrotations) (`Timeline|LockerOpening` :!via `PlayFromStart`)
        (:`Update`
          (`SceneComponent.K2_SetRelativeRotation` (`self.Door`) (`KismetMathLibrary.MakeRotator` 0.0 0.0 _doorrotations) false false))))))

(fn `ReceiveEvent`
  (params (CalledTag :type "GameplayTag Structure") (CallingObject :type "Object Object Reference (by ref)"))
  (returns (Return :type Boolean))
  (`|SwitchGameplayTag` CalledTag
    (:`Event.Locker.Open`
      (if (`self.isLockedInInteraction`)
        (set `self.isLockedInInteraction` false)
        (`self.OpenDoor`)
        (else
          (return false))))))

(fn `UserConstructionScript`
  (`parent.UserConstructionScript`))