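; A destructible light panel with three bulb meshes and a spotlight that can be switched on and off.
; BeginPlay caches bulb materials and spotlight intensity, which TurnLightsOn restores.
; TurnLightsOff zeroes the intensity and applies an unlit-bulb material to bulbs flagged in LightsON.
; Any damage to its Health component spawns sparks and replaces the actor with a plain movable copy of the panel mesh.
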(event `self.ReceiveBeginPlay`
  (`KismetArrayLibrary.Array_Add` (`self.Materials`) (`PrimitiveComponent.GetMaterial` (`self.Sphere_0`) 0))
  (`KismetArrayLibrary.Array_Add` (`self.Materials`) (`PrimitiveComponent.GetMaterial` (`self.Sphere_1`) 0))
  (`KismetArrayLibrary.Array_Add` (`self.Materials`) (`PrimitiveComponent.GetMaterial` (`self.Sphere_2`) 0))
  (set `self.AmbiantLightIntensity` (`LightComponentBase.Intensity` (`self.SpotLight`))))

(event `TurnLightsOff`
  (`self.RemoveEmissiveMaterials`)
  (`LightComponent.SetIntensity` (`self.SpotLight`) 0.0))

(event `TurnLightsOn`
  (`self.ResetMaterials`)
  (`LightComponent.SetIntensity` (`self.SpotLight`) (`self.AmbiantLightIntensity`)))

(event `self.Health.OnDamage`
  (params (DamageContext :type "DamageContext Structure (by ref)"))
  (`NiagaraFunctionLibrary.SpawnSystemAtLocation` "/Game/Art/VFX/NS_Sparks/NS_Sparks_Lock_Shoot.NS_Sparks_Lock_Shoot" (`SceneComponent.K2_GetComponentLocation` (`self.PanelLight`)))
  (bind _returnvalue (`|SpawnActorFromClass` "/Script/Engine.StaticMeshActor" (`SceneComponent.K2_GetComponentToWorld` (`self.PanelLight`)) "AlwaysSpawn" "MultiplyWithRoot" null null))
  (`StaticMeshActor.SetMobility` _returnvalue "Movable")
  (`StaticMeshComponent.SetStaticMesh` (`StaticMeshActor.StaticMeshComponent` _returnvalue) (`StaticMeshComponent.StaticMesh` (`self.PanelLight`)))
  (`self.K2_DestroyActor`))

(fn `RemoveEmissiveMaterials`
  (`|ExecutionSequence`
    (:`then_0`
      (if (`|GetArrayItem` (`self.LightsON`))
        (bind _sphere_0 (`self.Sphere_0`)
          (:`then`
            (`PrimitiveComponent.SetMaterial` _sphere_0 0 "/Game/Design/GPE/Destructible/Lights/MI_BulbTEST.MI_BulbTEST"))
          (:`else`))))
    (:`then_1`
      (if (`|GetArrayItem` (`self.LightsON`) 1)
        (bind _sphere_1 (`self.Sphere_1`)
          (:`then`
            (`PrimitiveComponent.SetMaterial` _sphere_1 0 "/Game/Design/GPE/Destructible/Lights/MI_BulbTEST.MI_BulbTEST"))
          (:`else`))))
    (:`then_2`
      (if (`|GetArrayItem` (`self.LightsON`) 2)
        (bind _sphere_2 (`self.Sphere_2`)
          (:`then`
            (`PrimitiveComponent.SetMaterial` _sphere_2 0 "/Game/Design/GPE/Destructible/Lights/MI_BulbTEST.MI_BulbTEST"))
          (:`else`))))))

(fn `ResetMaterials`
  (`|ExecutionSequence`
    (:`then_0`
      (bind _sphere_0 (`self.Sphere_0`)
        (:`then`
          (`PrimitiveComponent.SetMaterial` _sphere_0 0 (`|GetArrayItem` (`self.Materials`))))
        (:`else`)))
    (:`then_1`
      (bind _sphere_1 (`self.Sphere_1`)
        (:`then`
          (`PrimitiveComponent.SetMaterial` _sphere_1 0 (`|GetArrayItem` (`self.Materials`) 1)))
        (:`else`)))
    (:`then_2`
      (bind _sphere_2 (`self.Sphere_2`)
        (:`then`
          (`PrimitiveComponent.SetMaterial` _sphere_2 0 (`|GetArrayItem` (`self.Materials`) 2)))
        (:`else`)))))

(fn `UserConstructionScript`
  (locals (LightCount :type Integer :default 3)))