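; Destructible three-bulb street lamp that can flicker and be switched on or off.
; A hit component's first tag selects the bulb, which is swapped for a vertex animation texture collapse driven by a timeline.
; Breaking the last lit bulb removes the ambient light, stops audio and unlocks CLAIR_OBSCUR, plus METRO when all normal achievements are done.
; Flicker and on/off functions swap bulb materials and adjust lights, largely guided by LightsON.
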(event `self.ReceiveBeginPlay`
  (`KismetArrayLibrary.Array_Add` (`self.Materials`) (`PrimitiveComponent.GetMaterial` (`self.Bulb_0`) 0))
  (`KismetArrayLibrary.Array_Add` (`self.Materials`) (`PrimitiveComponent.GetMaterial` (`self.Bulb_1`) 0))
  (`KismetArrayLibrary.Array_Add` (`self.Materials`) (`PrimitiveComponent.GetMaterial` (`self.Bulb_2`) 0))
  (set `self.AmbiantLightIntensity` (`LightComponentBase.Intensity` (`self.AmbiantLight`)))
  (for _array_element (`self.LightsON`)
    (if _array_element
      (`/Engine/EditorBlueprintResources/StandardMacros.IncrementInt` (`self.LightBulbLeft`)
        (:`  `
          (bind _asbp_metro_game_instance (cast `/Game/Design/_GameManagement/Core/BP_MetroGameInstance` (`GameplayStatics.GetGameInstance`)))
          (set `self.Game Instance` _asbp_metro_game_instance))))))

(event `OnBulbDestroyed`
  (bind _returnvalue (`GameplayStatics.GetPlayerController` 0))
  (bind _returnvalue_2 (`GameplayStatics.GetPlayerController` 0))
  (bind _game_instance (`self.Game Instance`))
  (bind _result (`/Engine/EditorBlueprintResources/StandardMacros.DecrementInt` (`self.LightBulbLeft`))
    (:`  `
      (if (== _result 0)
        (`ActorComponent.K2_DestroyComponent` (`self.AmbiantLight`))
        (`AudioComponent.Stop` (`self.Audio`))
        ;[0 1 0.8795 0.33] ACHIEVEMENT : CLAIR OBSCUR
        (`AchievementQueryCallbackProxy.CacheAchievements` _returnvalue
          (:`OnSuccess`
            (bind (_bfoundid _progress) (`AchievementBlueprintLibrary.GetCachedAchievementProgress` _returnvalue "CLAIR_OBSCUR"))
            (if _bfoundid
              (if (> _progress 0.0)
                (`KismetSystemLibrary.PrintString` "Achievements already unlocked !" true true (struct :`G` 1.0 :`B` 0.012183 :`A` 1.0) 6.0)
                (else
                  (`AchievementWriteCallbackProxy.WriteAchievementProgress` _returnvalue "CLAIR_OBSCUR"
                    (:`OnSuccess`
                      (`KismetSystemLibrary.PrintString` "Achievement unlocked !" true true (struct :`G` 1.0 :`B` 0.96591 :`A` 1.0) 6.0)
                      (set `/Game/Design/_GameManagement/Core/BP_MetroGameInstance.AchievementsUnlocked` (+ (`/Game/Design/_GameManagement/Core/BP_MetroGameInstance.AchievementsUnlocked` _game_instance) 1) _game_instance)
                      (if (== (`/Game/Design/_GameManagement/Core/BP_MetroGameInstance.AchievementsUnlocked` _game_instance) (`/Game/Design/_GameManagement/Core/BP_MetroGameInstance.TotalNormalAchievements` _game_instance))
                        (bind (_bfoundid_2 _progress_2) (`AchievementBlueprintLibrary.GetCachedAchievementProgress` _returnvalue_2 "METRO"))
                        (if _bfoundid_2
                          (if (> _progress_2 0.0)
                            (`KismetSystemLibrary.PrintString` "Achievements already unlocked !" true true (struct :`G` 1.0 :`B` 0.012183 :`A` 1.0) 10.0)
                            (else
                              (`AchievementWriteCallbackProxy.WriteAchievementProgress` _returnvalue_2 "METRO")))
                          (else
                            (`KismetSystemLibrary.PrintString` "Didn't find ID" true true (struct :`R` 1.0 :`G` 0.408724 :`A` 1.0) 10.0))))))))
              (else
                (`KismetSystemLibrary.PrintString` "Didn't find ID" true true (struct :`R` 1.0 :`G` 0.408724 :`A` 1.0) 6.0))))
          (:`OnFailure`
            (`KismetSystemLibrary.PrintString` "Couldn't cache achievements !" true true (struct :`R` 1.0 :`A` 1.0) 6.0)))))))

(event `PLAY VAT`
  (params (TargetVAT :type Integer))
  ;[1 1 1 0.33] NEED REFACTOR
  (`self.OnBulbDestroyed`)
  (switch `int` TargetVAT
    (:`0`
      (`GameplayStatics.PlaySoundAtLocation` "/Game/Sounds/Audio/SD/MetaSounds/MS_Sources/GPE/Lights_Collapse/MS_Lights_Collapse.MS_Lights_Collapse" (`SceneComponent.K2_GetComponentLocation` (`self.Light_Bulb0`)) (struct) 1.0 1.0 0.0 null null null null)
      (`ActorComponent.K2_DestroyComponent` (`self.Bulb_0`))
      (`ActorComponent.K2_DestroyComponent` (`self.Light_Bulb0`))
      (`SceneComponent.SetHiddenInGame` (`self.VAT_Bulb_0`) false false)
      (bind (_direction _animation) (`Timeline|Timeline` :!via `PlayFromStart`)
        (:`Update`
          (`MeshComponent.SetScalarParameterValueOnMaterials` (`self.VAT_Bulb_0`) "Display Frame" (+ (* _animation 239.0) 1.0)))))
    (:`1`
      (`GameplayStatics.PlaySoundAtLocation` "/Game/Sounds/Audio/SD/MetaSounds/MS_Sources/GPE/Lights_Collapse/MS_Lights_Collapse.MS_Lights_Collapse" (`SceneComponent.K2_GetComponentLocation` (`self.Light_Bulb1`)) (struct) 1.0 1.0 0.0 null null null null)
      (`ActorComponent.K2_DestroyComponent` (`self.Bulb_1`))
      (`ActorComponent.K2_DestroyComponent` (`self.Light_Bulb1`))
      (`SceneComponent.SetHiddenInGame` (`self.VAT_Bulb_1`) false false)
      (bind (_direction_2 _animation_2) (`Timeline|Timeline_0` :!via `PlayFromStart`)
        (:`Update`
          (`MeshComponent.SetScalarParameterValueOnMaterials` (`self.VAT_Bulb_1`) "Display Frame" (+ (* _animation_2 239.0) 1.0)))))
    (:`2`
      (`GameplayStatics.PlaySoundAtLocation` "/Game/Sounds/Audio/SD/MetaSounds/MS_Sources/GPE/Lights_Collapse/MS_Lights_Collapse.MS_Lights_Collapse" (`SceneComponent.K2_GetComponentLocation` (`self.Light_Bulb2`)) (struct) 1.0 1.0 0.0 null null null null)
      (`ActorComponent.K2_DestroyComponent` (`self.Bulb_2`))
      (`ActorComponent.K2_DestroyComponent` (`self.Light_Bulb2`))
      (`SceneComponent.SetHiddenInGame` (`self.VAT_Bulb_2`) false false)
      (bind (_direction_3 _animation_3) (`Timeline|Timeline_1` :!via `PlayFromStart`)
        (:`Update`
          (`MeshComponent.SetScalarParameterValueOnMaterials` (`self.VAT_Bulb_2`) "Display Frame" (+ (* _animation_3 239.0) 1.0)))))))

(event `TurnLightsOff`
  (bind _lightson (`self.LightsON`))
  (`self.RemoveEmissiveMaterials`)
  (`LightComponent.SetIntensity` (`self.AmbiantLight`) 0.0)
  (`GameplayStatics.PlaySoundAtLocation` "/Game/Sounds/Audio/SFX/SFX_GPE/SFX_ElecSparks/SC_ElecSpark.SC_ElecSpark" (`self.K2_GetActorLocation`) (struct) 1.0 1.0 0.0 "/Game/Sounds/Attenuations/SA_Default.SA_Default" null null null)
  (`SceneComponent.SetVisibility` (`self.Light_Bulb2`) false false)
  (`SceneComponent.SetVisibility` (`self.Light_Bulb0`) false false)
  (`SceneComponent.SetVisibility` (`self.Light_Bulb1`) false false)
  (`SceneComponent.SetVisibility` (`self.AmbiantLight`) false false)
  (for (_ _array_index) _lightson
    (`KismetArrayLibrary.Array_Set` _lightson _array_index)))

(event `TurnOnLights`
  (bind _lightson (`self.LightsON`))
  (`self.ResetMaterials`)
  (`LightComponent.SetIntensity` (`self.AmbiantLight`) (`self.AmbiantLightIntensity`))
  (`SceneComponent.SetVisibility` (`self.Light_Bulb2`) true false)
  (`SceneComponent.SetVisibility` (`self.Light_Bulb0`) true false)
  (`SceneComponent.SetVisibility` (`self.Light_Bulb1`) true false)
  (`SceneComponent.SetVisibility` (`self.AmbiantLight`) true false)
  (for (_ _array_index) _lightson
    (`KismetArrayLibrary.Array_Set` _lightson _array_index true)))

(fn `CanCallTakeDamage`
  (params (DamageContext :type "DamageContext Structure (by ref)"))
  (returns (ReturnValue :type Boolean))
  (return true))

(fn `IsShownAsDamageableToPlayer`
  (params (DamageType :type "EDamageType Enum" :default "Generic") (HitResult :type "HitResult Structure (by ref)"))
  (returns (ReturnValue :type Boolean))
  (return false))

(fn `OnFlickLightStart`
  (params (LightData :type "LightData Structure (by ref)"))
  (`self.RemoveEmissiveMaterials`)
  (setmembers `LightData` :`StructRef` LightData :`OriginalLightIntensity` (`self.AmbiantLightIntensity`)))

(fn `OnFlickLightStop`
  (params (LightData :type "LightData Structure (by ref)"))
  (`self.ResetMaterials`)
  (`|ExecutionSequence`
    (:`then_0`
      (bind _light_bulb0 (`self.Light_Bulb0`)
        (:`then`
          (`LightComponent.SetIntensity` _light_bulb0 0.0))
        (:`else`)))
    (:`then_1`
      (bind _light_bulb2 (`self.Light_Bulb2`)
        (:`then`
          (`LightComponent.SetIntensity` _light_bulb2 0.0))
        (:`else`)))
    (:`then_2`
      (bind _light_bulb1 (`self.Light_Bulb1`)
        (:`then`
          (`LightComponent.SetIntensity` _light_bulb1 0.0))
        (:`else`)))
    (:`then_3`
      (return))))

(fn `OnFlickLightTick`
  (params (DeltaTime :type "Float (single-precision)") (LightData :type "LightData Structure (by ref)"))
  (return))

(fn `OnFlickLightUpdate`
  (params (LightData :type "LightData Structure (by ref)") (IntensityScale :type "Float (single-precision)"))
  (bind _returnvalue (* (`KismetMathLibrary.RandomFloatInRange` 3.0 10.0) IntensityScale))
  (`|ExecutionSequence`
    (:`then_0`
      (bind _bulb_0 (`self.Bulb_0`)
        (:`then`
          (if (`|GetArrayItem` (`self.LightsON`))
            (`MeshComponent.SetScalarParameterValueOnMaterials` _bulb_0 "Emissive Intensity" _returnvalue)))
        (:`else`)))
    (:`then_1`
      (bind _bulb_1 (`self.Bulb_1`)
        (:`then`
          (if (`|GetArrayItem` (`self.LightsON`) 1)
            (`MeshComponent.SetScalarParameterValueOnMaterials` _bulb_1 "Emissive Intensity" _returnvalue)))
        (:`else`)))
    (:`then_2`
      (bind _bulb_2 (`self.Bulb_2`)
        (:`then`
          (if (`|GetArrayItem` (`self.LightsON`) 2)
            (`MeshComponent.SetScalarParameterValueOnMaterials` _bulb_2 "Emissive Intensity" _returnvalue)))
        (:`else`)))
    (:`then_3`
      (return))))

(fn `RemoveEmissiveMaterials`
  (`|ExecutionSequence`
    (:`then_0`
      (if (`|GetArrayItem` (`self.LightsON`))
        (bind _bulb_0 (`self.Bulb_0`)
          (:`then`
            (`PrimitiveComponent.SetMaterial` _bulb_0 0 "/Game/Art/0_Materials/M_Emissive_Bulb_retake_03.M_Emissive_Bulb_retake_03"))
          (:`else`))))
    (:`then_1`
      (if (`|GetArrayItem` (`self.LightsON`) 1)
        (bind _bulb_1 (`self.Bulb_1`)
          (:`then`
            (`PrimitiveComponent.SetMaterial` _bulb_1 0 "/Game/Art/0_Materials/M_Emissive_Bulb_retake_03.M_Emissive_Bulb_retake_03"))
          (:`else`))))
    (:`then_2`
      (if (`|GetArrayItem` (`self.LightsON`) 2)
        (bind _bulb_2 (`self.Bulb_2`)
          (:`then`
            (`PrimitiveComponent.SetMaterial` _bulb_2 0 "/Game/Art/0_Materials/M_Emissive_Bulb_retake_03.M_Emissive_Bulb_retake_03"))
          (:`else`))))))

(fn `ResetMaterials`
  (`|ExecutionSequence`
    (:`then_0`
      (bind _bulb_0 (`self.Bulb_0`)
        (:`then`
          (if (`|GetArrayItem` (`self.LightsON`))
            (`PrimitiveComponent.SetMaterial` _bulb_0 0 (`|GetArrayItem` (`self.Materials`)))))
        (:`else`)))
    (:`then_1`
      (bind _bulb_1 (`self.Bulb_1`)
        (:`then`
          (if (`|GetArrayItem` (`self.LightsON`) 1)
            (`PrimitiveComponent.SetMaterial` _bulb_1 0 (`|GetArrayItem` (`self.Materials`) 1))))
        (:`else`)))
    (:`then_2`
      (bind _bulb_2 (`self.Bulb_2`)
        (:`then`
          (if (`|GetArrayItem` (`self.LightsON`) 2)
            (`PrimitiveComponent.SetMaterial` _bulb_2 0 (`|GetArrayItem` (`self.Materials`) 2))))
        (:`else`)))))

(fn `RetrieveFlickableLights`
  (returns (ReturnValue :type "Array of LightComponent Object Reference"))
  (locals (FlickableLights :type "Array of LightComponent Object Reference"))
  (bind _flickablelights (`local.FlickableLights`))
  (`|ExecutionSequence`
    (:`then_0`
      (if (`|GetArrayItem` (`self.LightsON`))
        (`KismetArrayLibrary.Array_Add` (`local.FlickableLights`) (`self.Light_Bulb0`))))
    (:`then_1`
      (if (`|GetArrayItem` (`self.LightsON`) 1)
        (`KismetArrayLibrary.Array_Add` (`local.FlickableLights`) (`self.Light_Bulb1`))))
    (:`then_2`
      (if (`|GetArrayItem` (`self.LightsON`) 2)
        (`KismetArrayLibrary.Array_Add` (`local.FlickableLights`) (`self.Light_Bulb2`))))
    (:`then_3`
      (`KismetArrayLibrary.Array_Add` _flickablelights (`self.AmbiantLight`))
      (return _flickablelights))))

(fn `TakeDamage`
  (params (DamageContext :type "DamageContext Structure (by ref)"))
  (returns (ReturnValue :type Boolean))
  (bind (_bblockinghit _binitialoverlap _time _distance _location _impactpoint _normal _impactnormal _physmat _hitactor _hitcomponent) (`GameplayStatics.BreakHitResult` (`.HitResult` (break `DamageContext` DamageContext))))
  (bind _componenttags (`ActorComponent.ComponentTags` _hitcomponent))
  (`/Engine/EditorBlueprintResources/StandardMacros.IsValid` _hitcomponent
    (:`Is Valid`
      (if (`KismetArrayLibrary.Array_IsNotEmpty` _componenttags)
        (`self.PLAY VAT` (`KismetStringLibrary.Conv_StringToInt` (`KismetStringLibrary.Conv_NameToString` (`|GetArrayItem` _componenttags))))))
    (:`Is Not Valid`
      _))
  (return false))

(fn `UserConstructionScript`)