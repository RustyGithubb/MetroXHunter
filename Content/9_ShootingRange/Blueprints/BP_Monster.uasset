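; BP_Monster is a shooting range enemy that chases the player and dies on reaching them or when any weak point dies.
; BeginPlay binds each weak point's LifeComponent death event, starts the animation and issues AIMoveTo toward the player pawn.
; A self-restarting timeline, alternated forward and reverse by FlipFlop, procedurally swings four legs and bobs body and head.
; While running, Tick launches it upward once the player is within jump range.
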(event `self.ReceiveTick`
  (params (DeltaSeconds :type "Float (single-precision)"))
  ;[1 0 0.005598 0.25] TICK
  ;;[1 1 1 0.33] Jump to Target
  (if (and (`self.bIsRunning`) (not (`self.bIsJumping`)))
    (if (<= (`self.GetDistanceTo` (`self.Target`) self) (`self.JumpRange`))
      (`self.LaunchCharacter` (0.0 0.0 500.0))
      (set `self.bIsJumping` true))))

(event `self.ReceiveBeginPlay`
  ;[1 0 0.005598 0.25] BEGIN PLAY
  (`parent.ReceiveBeginPlay`)
  ;;[1 1 1 0.33] Bind WeakPoint's LifeComponent Event OnDeath
  (for _array_element (`self.WeakPoints`)
    (add `/Game/0_Design/LifeSystem/BP_LifeComponent.OnDeath` (`/Game/0_Design/EyeVisionSystem/BP_WeakPoints.LifeComponent` _array_element) (delegate `OnWeakPointDown`))
    (`self.RunAnimation`)
    (bind _output_get (set `self.Target` (`GameplayStatics.GetPlayerPawn` 0)))
    (`|AIMoveTo` self (0.0 0.0 0.0) _output_get
      (:`OnSuccess`
        (`self.OnDeath`)
        (`self.K2_DestroyActor`)))))

(event `OnWeakPointDown`
  ;[1 0 0.005598 0.25] BEGIN PLAY
  (`self.OnDeath`)
  (`self.K2_DestroyActor`))

(event `RunAnimation`
  ;[0.2135 1 0 0.25] RUN ANIMATION
  (if (`self.bIsRunning`)
    (`/Engine/EditorBlueprintResources/StandardMacros.FlipFlop`
      (:`A`
        (bind (_direction _rotation _delayedrotation _bouncybody) (`Timeline|LegsAnimations` :!via `PlayFromStart` :!label _label)
          (:`Update`
            (`|ExecutionSequence`
              (:`then_0`
                (bind _returnvalue (* _rotation 20.0))
                (`SceneComponent.K2_SetRelativeRotation` (`self.LFrontLeg`) (`KismetMathLibrary.MakeRotator` _returnvalue 20.0 -90.0) false false)
                (`SceneComponent.K2_SetRelativeRotation` (`self.LBackLeg`) (`KismetMathLibrary.MakeRotator` (* _returnvalue -1.0) 20.0 -90.0) false false))
              (:`then_1`
                (bind _returnvalue_2 (* _delayedrotation 20.0))
                (`SceneComponent.K2_SetRelativeRotation` (`self.RBackLeg`) (`KismetMathLibrary.MakeRotator` (* _returnvalue_2 -1.0) 20.0 90.0) false false)
                (`SceneComponent.K2_SetRelativeRotation` (`self.RFrontLeg`) (`KismetMathLibrary.MakeRotator` _returnvalue_2 20.0 90.0) false false))
              (:`then_2`
                (bind _returnvalue_3 (* _bouncybody 2.0))
                (`SceneComponent.K2_SetRelativeLocation` (`self.Body`) (`KismetMathLibrary.MakeVector` 0.0 0.0 (+ _returnvalue_3 -18.0)) false false)
                (`SceneComponent.K2_SetRelativeLocation` (`self.Head`) (`KismetMathLibrary.MakeVector` 30.0 0.0 (+ (* _returnvalue_3 -1.0) -17.0)) false false))))
          (:`Finished`
            (`self.RunAnimation`))))
      (:`B`
        (goto _label :!via `ReverseFromEnd`)))))

(fn `UserConstructionScript`
  (`parent.UserConstructionScript`))