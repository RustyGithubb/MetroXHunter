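; Trigger receiver component that plays a timed black screen fade and text fade when its trigger event fires.
; OnPlayComponentSpecificEvent starts LoadFade and LoadFadeText back to back with fixed durations.
; Each drives the BlackFader in the BP_MetroHUD viewport, fading in, waiting its own configurable delay, then fading out.
; LoadFadeText has no cast of its own and reuses the HUD reference from LoadFade.
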(event `LoadFade`
  (params (FadeInTime :type "Float (double-precision)" :default 3.0) (FadeOutTime :type "Float (double-precision)" :default 3.0))
  (bind _asbp_metro_hud (cast `/Game/Design/_GameManagement/Core/BP_MetroHUD` (`PlayerController.GetHUD` (`GameplayStatics.GetPlayerController` 0))))
  (bind _blackfader (`/Game/Design/Widgets/WBP_Viewport.BlackFader` (`/Game/Design/_GameManagement/Core/BP_MetroHUD.Viewport` _asbp_metro_hud)))
  (`/Game/Design/Widgets/WBP_BlackFader.Fade` _blackfader FadeInTime true)
  (`KismetSystemLibrary.Delay` (`self.WaitingTimeFade`))
  (`/Game/Design/Widgets/WBP_BlackFader.Fade` _blackfader FadeOutTime false))

(event `LoadFadeText`
  (params (FadeInText :type "Float (double-precision)" :default 3.0) (FadeOutText :type "Float (double-precision)" :default 3.0))
  (bind _blackfader (`/Game/Design/Widgets/WBP_Viewport.BlackFader` (`/Game/Design/_GameManagement/Core/BP_MetroHUD.Viewport` (stale `LoadFade` _asbp_metro_hud))))
  (`/Game/Design/Widgets/WBP_BlackFader.FadeText` _blackfader FadeInText true)
  (`KismetSystemLibrary.Delay` (`self.WaitingTimeText`))
  (`/Game/Design/Widgets/WBP_BlackFader.FadeText` _blackfader FadeOutText false))

(fn `OnPlayComponentSpecificEvent`
  (params (FromBoxEnter :type Boolean) (TriggerBox :type "Actor Object Reference"))
  (`self.LoadFade` 3.0)
  (`self.LoadFadeText` 3.0))