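; Trigger receiver component that gradually shifts the color of lights on assigned actors to a final color.
; On BeginPlay it caches every light component and its starting color, printing errors for missing actors or lights.
; The trigger event enables Tick, which lerps each light toward the target over the transition time.
; At the end it only disables Tick, without applying the exact final color or resetting the timer.
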(event `self.ReceiveBeginPlay`
  (`self.SetComponentTickEnabled` false)
  (if (`KismetArrayLibrary.Array_IsNotEmpty` (`self.ActorsThatShouldChange`))
    (`self.RegisterAllLights`)
    (else
      ;[0.0625 0.001432 0 0.33] ERROR PRINT
      (`KismetSystemLibrary.PrintText` (`|FormatText` "LightColorChangerComponent on Actor {actorName} \nhas not been given Actors to change. \nPlease Add one." (`KismetSystemLibrary.GetDisplayName` (`self.GetOwner`))) true true (struct :`R` 1.0 :`A` 1.0) 500.0))))

(event `self.ReceiveTick`
  (params (DeltaSeconds :type "Float (single-precision)"))
  (bind _return (`/Game/o_Libraries/BPL_GeneralUtilities.Increase Value Float` (`self.CurrentChangeTime`) (* (`GameplayStatics.GetWorldDeltaSeconds`) (`GameplayStatics.GetGlobalTimeDilation`))))
  (if (>= _return (`self.TransitionTime`))
    (`self.StopColorChange`)
    (else
      (`self.UpdateAllLights`))))

(fn `OnPlayComponentSpecificEvent`
  (params (FromBoxEnter :type Boolean))
  (`self.SetComponentTickEnabled` true))

(fn `RegisterAllLights`
  (locals (CurrentlyEvaluatedLights :type "Array of LightComponent Object Reference"))
  (`KismetArrayLibrary.Array_Clear` (`self.StartingLightColors`))
  (`KismetArrayLibrary.Array_Clear` (`self.LightsToFlicker`))
  ;[0.1724 0.05414 0.1771 0.33] Loop through all given Actors and get all of their Lights (if they have any!!)
  (for _array_element (`self.ActorsThatShouldChange`)
    (bind _output_get (set `local.CurrentlyEvaluatedLights` (`Actor.K2_GetComponentsByClass` _array_element "/Script/Engine.LightComponent")))
    (if (`KismetArrayLibrary.Array_IsNotEmpty` _output_get)
      ;[0.1979 0.08918 0.04725 0.33] Register each Light with their Starting Color
      (for _array_element_2 (`local.CurrentlyEvaluatedLights`)
        (`KismetArrayLibrary.Array_Add` (`self.LightsToFlicker`) _array_element_2)
        (`KismetArrayLibrary.Array_Add` (`self.StartingLightColors`) (`LightComponentBase.GetLightColor` _array_element_2)))
      (else
        ;[0.1927 0 0 0.33] ERROR PRINT
        (`KismetSystemLibrary.PrintText` (`|FormatText` "LightColorChangerComponent on Actor {actorName} \nhas been given Actor {fakeLight}, but it doesn't have any Light Components. \nPlease remove the Actor or add a Light to it." (`KismetSystemLibrary.GetDisplayName` (`self.GetOwner`)) (`KismetSystemLibrary.GetDisplayName` _array_element)) true true (struct :`R` 1.0 :`A` 1.0) 500.0)))))

(fn `StopColorChange`
  (`self.SetComponentTickEnabled` false))

(fn `UpdateAllLights`
  (locals (CurrentLight :type "LightComponent Object Reference") (NormalizedProgress :type "Float (double-precision)"))
  (set `local.NormalizedProgress` (/ (`self.CurrentChangeTime`) (`self.TransitionTime`)))
  (for (_array_element _array_index) (`self.LightsToFlicker`)
    (set `local.CurrentLight` _array_element)
    (`LightComponent.SetLightColor` (`local.CurrentLight`) (`KismetMathLibrary.LinearColorLerp` (`|GetArrayItem` (`self.StartingLightColors`) _array_index) (`self.FinalColor`) (`local.NormalizedProgress`)) true)))