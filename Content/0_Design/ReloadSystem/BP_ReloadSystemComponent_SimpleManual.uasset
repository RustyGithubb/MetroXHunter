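; Reload system component for simple manual reloading, where each reload input press adds one bullet to the gun's magazine.
; Loading works only while the player is aiming, the magazine is not full and the per-bullet load delay has elapsed.
; The same timestamp, extended by an additional lock time, reports when gun fire is locked.
; It creates its reload widget at BeginPlay, passing itself in, and removes it at EndPlay.
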(event `self.ReceiveBeginPlay`
  (bind _returnvalue (`|CreateWidget` "/Game/UI/Widgets/WBP_ReloadSystem_SimpleManual.WBP_ReloadSystem_SimpleManual_C" (cast `/Game/0_Design/GameManagement_/BPC_Controller` (`Pawn.GetController` (`self.PlayerCharacter`)) :!pure true) self))
  (bind _output_get (set `self.Widget` _returnvalue))
  (`UserWidget.AddToViewport` _output_get 0))

(event `self.ReceiveEndPlay`
  (params (EndPlayReason :type "EEndPlayReason Enum" :default "Destroyed"))
  (`Widget.RemoveFromParent` (`self.Widget`)))

(fn `CanInput`
  (params (`Additional Input Time` :type "Float (double-precision)"))
  (returns (`Can Input` :type Boolean))
  (return (<= (- (+ (`self.NextInputTime`) `Additional Input Time`) (`KismetSystemLibrary.GetGameTimeInSeconds`)) 0.0)))

(fn `CanReload`
  (returns (CanReload :type Boolean))
  (return (and (`/Game/0_Design/GameManagement_/BP_MainChara.Aiming` (`self.PlayerCharacter`)) (`self.CanInput` 0.0) (not (`/Game/0_Design/GameManagement_/BP_Gun.IsGunFull` (`self.Gun`))))))

(fn `IsLockingGunFire`
  (returns (IsFireLocked :type Boolean))
  (return (not (`self.CanInput` (`self.AdditionalFireLockTime`)))))

(fn `OnReloadInput`
  (params (`Input Type` :type "/Game/0_Design/E_InputActionType Enum" :default "NewEnumerator0"))
  (bind _loadbullettime (`self.LoadBulletTime`))
  (switch `/Game/0_Design/E_InputActionType` `Input Type`
    (:`NewEnumerator1`
      ;[1 1 1 0.33] Check can reload
      (if (`self.CanReload`)
        ;[1 1 1 0.33] Add a bullet into magazine
        (`/Engine/EditorBlueprintResources/StandardMacros.IncrementInt` (`/Game/0_Design/GameManagement_/BP_Gun.IndexMagazineAmmo` (`self.Gun`))
          (:`  `
            ;[1 1 1 0.33] Delay next input time
            (set `self.NextInputTime` (+ (`KismetSystemLibrary.GetGameTimeInSeconds`) _loadbullettime))
            (`KismetSystemLibrary.PrintText` (`|FormatText` "ReloadSystem: add a bullet and delay for {Time}s" _loadbullettime))))
        (else
          (`KismetSystemLibrary.PrintString` "ReloadSystem: Can't reload!" true true (struct :`R` 1.0 :`A` 1.0) 2.0 "ReloadSystemCantReload"))))))