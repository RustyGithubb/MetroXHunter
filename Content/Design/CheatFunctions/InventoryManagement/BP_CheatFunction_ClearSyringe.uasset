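; Cheat function that clears the syringe segments in the player's inventory.
; On init it waits a tick, then caches the InventoryComponent from the pawn controlled by the cheat manager's player controller.
; When the cheat fires, it calls ClearSyringeSegments on that cached component if it is valid.
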(event `self.OnInit`
  (`KismetSystemLibrary.DelayUntilNextTick`)
  (`self.RegisterInventoryComponent`))

(event `self.OnCheat`
  (bind _playerinventory (`self.PlayerInventory`)
    (:`then`
      (`InventoryComponent.ClearSyringeSegments` _playerinventory))
    (:`else`)))

(fn `RegisterInventoryComponent`
  (bind _returnvalue (`Controller.K2_GetPawn` (`CheatManager.GetPlayerController` (`self.CheatManager`))))
  (`/Engine/EditorBlueprintResources/StandardMacros.IsValid` _returnvalue
    (:`Is Valid`
      (set `self.PlayerInventory` (`Actor.GetComponentByClass` _returnvalue "/Script/MetroXHunter.InventoryComponent")))))