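; BP_FakeInfected is a gameplay prop standing in for an infected, with a skeletal mesh that reacts physically to gunfire.
; On bullet damage from its Health component, it sets the linear velocity of all physics bodies along the shot trace, replacing their current velocity.
; It then hides the hit bone unless that bone is listed in NonDestroyableBones, so body parts can be shot off.
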(event `self.Health.OnDamage`
  (params (DamageContext :type "DamageContext Structure (by ref)"))
  (bind (_healthcomponent _damageamount _damagetype _attackeractor _inflictoractor _hitresult) (break `DamageContext` DamageContext))
  (bind (_bblockinghit _binitialoverlap _time _distance _location _impactpoint _normal _impactnormal _physmat _hitactor _hitcomponent _hitbonename _bonename _hititem _elementindex _faceindex _tracestart _traceend) (`GameplayStatics.BreakHitResult` _hitresult))
  (switch `EDamageType` _damagetype
    (:`Bullet`
      (`PrimitiveComponent.SetAllPhysicsLinearVelocity` (`self.SkeletalMeshComponent`) (* (`KismetMathLibrary.GetDirectionUnitVector` _tracestart _traceend) 300.0) false)
      (if (not (`BlueprintSetLibrary.Set_Contains` (`self.NonDestroyableBones`) _hitbonename))
        (`GameplayLibrary.SetBoneHidden` (`self.SkeletalMeshComponent`) _hitbonename)))))

(fn `UserConstructionScript`)