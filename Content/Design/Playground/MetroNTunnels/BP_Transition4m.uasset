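; Modular 4m metro tunnel transition piece whose ceiling, side walls, door and stairs-or-floor layout are configured by boolean flags.
; The construction script and BeginPlay apply the flags, toggling meshes and resizing the floor where it replaces stairs.
; Helper functions switch visibility, collision and navigation relevance together.
; At BeginPlay, a false WithoutDoor re-enables the door even when ReplaceDoorByWall has hidden it.
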(event `self.ReceiveBeginPlay`
  (bind _sm_floor_4x4 (`self.SM_Floor_4x4`))
  (bind _sm_floor_4x4_2 (`self.SM_Floor_4x4`))
  (if (`self.CutCeiling`)
    (`self.DisableCollisionAndVisibility` (`|MakeArray` (`self.SM_Ceiling_4x4`)))
    (else
      (`self.EnableCollisionAndVisibility` (`|MakeArray` (`self.SM_Ceiling_4x4`)))))
  (if (`self.CutLeftHalf`)
    (`self.DisableCollisionAndVisibility` (`|MakeArray` (`self.SM_L_Wall_4x4`))))
  (if (`self.CutRightHalf`)
    (`self.DisableCollisionAndVisibility` (`|MakeArray` (`self.SM_R_Wall_4x4`))))
  (if (`self.ReplaceDoorByWall`)
    (`self.DisableCollisionAndVisibility` (`|MakeArray` (`self.SM_Door_4x0_5x4`)))
    (`self.EnableCollisionAndVisibility` (`|MakeArray` (`self.SM_T_Wall_4x4`)))
    (else
      (`self.DisableCollisionAndVisibility` (`|MakeArray` (`self.SM_T_Wall_4x4`)))))
  (if (`self.WithoutDoor`)
    (`self.DisableCollisionAndVisibility` (`|MakeArray` (`self.SM_Door_4x0_5x4`)))
    (else
      (`self.EnableCollisionAndVisibility` (`|MakeArray` (`self.SM_Door_4x0_5x4`)))))
  (if (`self.ReplaceStairsByFloor`)
    (`SceneComponent.K2_SetRelativeLocation` _sm_floor_4x4_2 (0.0 -100.0 0.0) false false)
    (`SceneComponent.SetRelativeScale3D` _sm_floor_4x4_2 (1.0 0.5 1.0))
    (else
      (`SceneComponent.K2_SetRelativeLocation` _sm_floor_4x4 (200.0 -100.0 0.0) false false)
      (`SceneComponent.SetRelativeScale3D` _sm_floor_4x4 (0.5 0.5 1.0)))))

(fn `DisableCollisionAndVisibility`
  (params (`Static Meshes` :type "Array of StaticMeshComponent Object Reference (by ref)") (Lights :type "Array of LightComponent Object Reference (by ref)"))
  ;[1 0.5264 0.4766 0.33] DisableSM
  (for _array_element `Static Meshes`
    (`SceneComponent.SetHiddenInGame` _array_element true false)
    (`SceneComponent.SetVisibility` _array_element false false)
    (`PrimitiveComponent.SetCollisionEnabled` _array_element "NoCollision")
    (`UtilityLibrary.SetActorComponentCanEverAffectNavigation` _array_element))
  ;[1 0.8982 0.4238 0.33] DisableLights
  (for _array_element_2 Lights
    (`SceneComponent.SetHiddenInGame` _array_element_2 true false)
    (`SceneComponent.SetVisibility` _array_element_2 false false)
    (`UtilityLibrary.SetActorComponentCanEverAffectNavigation` _array_element_2))
  (return))

(fn `EnableCollisionAndVisibility`
  (params (`Static Meshes` :type "Array of StaticMeshComponent Object Reference") (Lights :type "Array of LightComponent Object Reference"))
  ;[1 0.5264 0.4766 0.33] DisableSM
  (for _array_element `Static Meshes`
    (`SceneComponent.SetHiddenInGame` _array_element false false)
    (`SceneComponent.SetVisibility` _array_element true false)
    (`PrimitiveComponent.SetCollisionEnabled` _array_element "QueryAndPhysics")
    (`UtilityLibrary.SetActorComponentCanEverAffectNavigation` _array_element true))
  ;[1 0.8982 0.4238 0.33] DisableLights
  (for _array_element_2 Lights
    (`SceneComponent.SetHiddenInGame` _array_element_2 false false)
    (`SceneComponent.SetVisibility` _array_element_2 true false)
    (`UtilityLibrary.SetActorComponentCanEverAffectNavigation` _array_element_2 true))
  (return))

(fn `UserConstructionScript`
  (bind _sm_floor_4x4 (`self.SM_Floor_4x4`))
  (bind _sm_floor_4x4_2 (`self.SM_Floor_4x4`))
  (if (`self.CutCeiling`)
    (`self.DisableCollisionAndVisibility` (`|MakeArray` (`self.SM_Ceiling_4x4`))))
  (if (`self.CutLeftHalf`)
    (`self.DisableCollisionAndVisibility` (`|MakeArray` (`self.SM_L_Wall_4x4`))))
  (if (`self.CutRightHalf`)
    (`self.DisableCollisionAndVisibility` (`|MakeArray` (`self.SM_R_Wall_4x4`))))
  (if (`self.ReplaceDoorByWall`)
    (`self.DisableCollisionAndVisibility` (`|MakeArray` (`self.SM_Door_4x0_5x4`)))
    (`self.EnableCollisionAndVisibility` (`|MakeArray` (`self.SM_T_Wall_4x4`)))
    (else
      (`self.DisableCollisionAndVisibility` (`|MakeArray` (`self.SM_T_Wall_4x4`)))))
  (if (`self.WithoutDoor`)
    (`self.DisableCollisionAndVisibility` (`|MakeArray` (`self.SM_Door_4x0_5x4`))))
  (if (`self.ReplaceStairsByFloor`)
    (`SceneComponent.K2_SetRelativeLocation` _sm_floor_4x4_2 (0.0 -100.0 0.0) false false)
    (`SceneComponent.SetRelativeScale3D` _sm_floor_4x4_2 (1.0 0.5 1.0))
    (else
      (`SceneComponent.K2_SetRelativeLocation` _sm_floor_4x4 (200.0 -100.0 0.0) false false)
      (`SceneComponent.SetRelativeScale3D` _sm_floor_4x4 (0.5 0.5 1.0)))))