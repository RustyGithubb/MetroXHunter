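; Toggleable cheat function that shows an on-screen diagram visualizing controller inputs, optionally enabled at game start.
; Toggling on lazily creates the visualizer widget, registers it on BPC_Controller, adds it to the viewport and adds a dedicated Enhanced Input mapping context.
; The mapping step retries each tick until the input subsystem is valid, an acknowledged workaround for BeginPlay timing.
; Toggling off removes both widget and context.
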(event `self.OnCheat`
  (bind _returnvalue (pcsubsystem `EnhancedInputLocalPlayerSubsystem` (`self.PlayerController`)))
  (if (`self.IsToggled`)
    (`self.VisualizerWidget`
      (:`then`
        _)
      (:`else`
        (`self.CreateWidget`)))
    (`UserWidget.AddToViewport` (`self.VisualizerWidget`) 0)
    ;[1 1 1 0.33] I know the "Delay until valid" is HORRIBLE, but on BeginPlay the Subsystem isn't valid...
    ; Sorry!!!
    (`/Engine/EditorBlueprintResources/StandardMacros.IsValid` _returnvalue :!label _label
      (:`Is Valid`
        (`EnhancedInputSubsystemInterface.AddMappingContext` _returnvalue "/Game/0_Design/GameManagement_/Input/Visualizer/IMC_ControllerVisualizer.IMC_ControllerVisualizer" 10 (make `ModifyContextOptions` false)))
      (:`Is Not Valid`
        (`KismetSystemLibrary.DelayUntilNextTick`)
        (goto _label)))
    (else
      (`Widget.RemoveFromParent` (`self.VisualizerWidget`))
      (`EnhancedInputSubsystemInterface.RemoveMappingContext` (pcsubsystem `EnhancedInputLocalPlayerSubsystem` (`self.PlayerController`)) "/Game/0_Design/GameManagement_/Input/Visualizer/IMC_ControllerVisualizer.IMC_ControllerVisualizer" (make `ModifyContextOptions` false)))))

(event `self.OnInit`
  (`|ExecutionSequence`
    (:`then_0`
      (bind _cheatmanager (`self.CheatManager`)
        (:`then`
          (bind _asbpc_controller (cast `/Game/0_Design/GameManagement_/BPC_Controller` (`CheatManager.GetPlayerController` _cheatmanager)))
          (set `self.PlayerController` _asbpc_controller))
        (:`else`)))
    (:`then_1`
      ;[1 1 1 0.33] Start the game with the diagram shown
      (if (`self.StartsEnabled`)
        (`self.Cheat` (make `MXHCheatFunctionActionParams` true))))))

(fn `CreateWidget`
  (bind _returnvalue (`|CreateWidget` "/Game/UI/Widgets/InputVisualizers/WBP_ControllerInputsVisualizer.WBP_ControllerInputsVisualizer_C"))
  (bind _output_get (set `self.VisualizerWidget` _returnvalue))
  (set `/Game/0_Design/GameManagement_/BPC_Controller.ControllerInputVisualizer` _output_get (`self.PlayerController`)))